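; Spline-based water stream Blueprint for the AnemonePlanet VFX, combining spline meshes with a Niagara water flow effect.
; The construction script passes the spline to the Niagara component's Splines variable, then adds a spline mesh per segment using point locations and tangents.
; The outer ends of the first and last segments are scaled up to flare the stream.
; All logic runs at construction, with an empty event graph.
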(event EventBeginPlay)

(event Collision|EventActorBeginOverlap
  (params (OtherActor :type Actor%20Object%20Reference)))

(event EventTick
  (params (DeltaSeconds :type Float%20%28single-precision%29)))

(fn ConstructionScript
  (bind _spline (Variables|Default|GetSpline))
  (bind _scale (Variables|Default|GetScale))
  (bind _spline_2 (Variables|Default|GetSpline))
  (bind _scale_2 (Variables|Default|GetScale))
  (bind _scale_3 (Variables|Default|GetScale))
  (bind _returnvalue (Spline|GetNumberOfSplinePoints _spline))
  (bind _returnvalue_2 (- _returnvalue 2))
  (Utilities|FlowControl|Sequence
    (:then_0
      (Class|NiagaraComponent|SetVariableObject (Variables|Default|GetNS_WaterFlow1) "Splines" (Variables|Default|GetSpline)))
    (:then_1
      (for _index (range 0 _returnvalue_2)
        (bind _returnvalue_3 (AddComponent|AddSplineMeshComponent false))
        (if (== _index 0)
          (Components|StaticMesh|SetStaticMesh _returnvalue_3 (Variables|Default|GetMesh))
          (SplineMesh|SetStartScale _returnvalue_3 (+ _scale_3 "(X=15.000000,Y=15.000000)") true :!class /Script/Engine.SplineMeshComponent)
          (SplineMesh|SetEndScale _returnvalue_3 _scale_3 true :!class /Script/Engine.SplineMeshComponent)
          (elif (== _index _returnvalue_2)
            (Components|StaticMesh|SetStaticMesh _returnvalue_3 (Variables|Default|GetMesh))
            (SplineMesh|SetStartScale _returnvalue_3 _scale true :!class /Script/Engine.SplineMeshComponent)
            (SplineMesh|SetEndScale _returnvalue_3 (+ _scale "(X=15.000000,Y=15.000000)") true :!class /Script/Engine.SplineMeshComponent)
            (else
              (Components|StaticMesh|SetStaticMesh _returnvalue_3 (Variables|Default|GetMesh))
              (SplineMesh|SetStartScale _returnvalue_3 _scale_2 true :!class /Script/Engine.SplineMeshComponent)
              (SplineMesh|SetEndScale _returnvalue_3 _scale_2 true :!class /Script/Engine.SplineMeshComponent))))
        (SplineMesh|SetStartandEnd _returnvalue_3 (Spline|GetLocationatSplinePoint _spline_2 _index "Local") (Spline|GetTangentatSplinePoint _spline_2 _index "Local") (Spline|GetLocationatSplinePoint _spline_2 (+ _index 1) "Local") (Spline|GetTangentatSplinePoint _spline_2 (+ _index 1) "Local") true :!class /Script/Engine.SplineMeshComponent)))))