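; BP_flow is a Niagara effect actor that passes its Spline component to the system's "Splines" variable, at construction and BeginPlay.
; It samples the spline at 100 constant-velocity steps, subtracting actor location from local-space points, to estimate a bounding box adjusted by BoundsOffset.
; The box is only printed, as the node setting the system's fixed bounds is disconnected.
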(event EventBeginPlay
  (CallFunction|NiagaraInitialize))

(event Collision|EventActorBeginOverlap
  (params (OtherActor :type Actor%20Object%20Reference)))

(event EventTick
  (params (DeltaSeconds :type Float%20%28single-precision%29)))

(fn ConstructionScript
  (CallFunction|NiagaraInitialize))

(fn NiagaraInitialize
  (Niagara|SetNiagaraVariable(Object) (Variables|Default|GetNiagara) "Splines" (Variables|Default|GetSpline))
  (bind (_min _max) (CallFunction|EstimateSplineBounds))
  (Development|PrintString (Utilities|String|ToString(Integer) (Math|Box|MakeBox _min _max))))

(fn EstimateSplineBounds
  (bind _boundsoffset (Variables|Default|GetBoundsOffset))
  (bind _output_get (LocalVariables|SetThisMin "100000000000.000000,100000000000.000000,100000000000.000000"))
  (LocalVariables|SetThisMax (* _output_get -1.0))
  (for _index (range 0 99)
    (bind _output_get_2 (LocalVariables|SetThisSample (- (Spline|GetLocationatTime (Variables|Default|GetSpline) (/ _index 100) "Local" true) (Transformation|GetActorLocation))))
    (LocalVariables|SetThisMin (Math|Vector|MakeVector (Math|Float|Min(Float) (.X (Math|Vector|BreakVector _output_get_2)) (.X (Math|Vector|BreakVector (LocalVariables|GetThisMin)))) (Math|Float|Min(Float) (.Y (Math|Vector|BreakVector _output_get_2)) (.Y (Math|Vector|BreakVector (LocalVariables|GetThisMin)))) (Math|Float|Min(Float) (.Z (Math|Vector|BreakVector _output_get_2)) (.Z (Math|Vector|BreakVector (LocalVariables|GetThisMin))))))
    (LocalVariables|SetThisMax (Math|Vector|MakeVector (Math|Float|Max(Float) (.X (Math|Vector|BreakVector _output_get_2)) (.X (Math|Vector|BreakVector (LocalVariables|GetThisMax)))) (Math|Float|Max(Float) (.Y (Math|Vector|BreakVector _output_get_2)) (.Y (Math|Vector|BreakVector (LocalVariables|GetThisMax)))) (Math|Float|Max(Float) (.Z (Math|Vector|BreakVector _output_get_2)) (.Z (Math|Vector|BreakVector (LocalVariables|GetThisMax)))))))
  (return (+ (LocalVariables|GetThisMin) _boundsoffset) (- (LocalVariables|GetThisMax) _boundsoffset)))