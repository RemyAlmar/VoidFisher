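; Animation notify that triggers a creature's flashbang effect, putting a flashbang overlay on the screens of actors seeing it.
; When fired, it casts the mesh owner to BP_CreatureGeneric and loops over the ActorSeeing list in its BPCPrey component.
; Each listed actor with a BPC_WidgetManager component gets UI_Flashbang added to the player screen through that component.
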(fn ReceivedNotify
  (params (MeshComp :type Skeletal%20Mesh%20Component%20Object%20Reference) (Animation :type Anim%20Sequence%20Base%20Object%20Reference) (EventReference :type Anim%20Notify%20Event%20Reference%20Structure%20%28by%20ref%29))
  (bind _asbp_creature_generic (Utilities|Casting|CastToBP_CreatureGeneric (Components|GetOwner MeshComp))
    (:then
      (LocalVariables|SetReceveid true)
      (for _array_element (Variables|/Game/Blueprints/AddOn/Components/BPC_Prey.BPC_Prey_C|GetActorSeeing (Variables|/Game/Blueprints/AI/Pawn/BP_CreatureGeneric.BP_CreatureGeneric_C|GetBPC_Prey _asbp_creature_generic))
        (Utilities|IsValid (Actor|GetComponentbyClass _array_element "/Game/Blueprints/AddOn/Components/BPC_WidgetManager.BPC_WidgetManager_C")
          (:Is%20Valid
            (Default|AddWidgettoPlayerScreen (Actor|GetComponentbyClass _array_element "/Game/Blueprints/AddOn/Components/BPC_WidgetManager.BPC_WidgetManager_C") "/Game/Blueprints/Widgets/Misc/UI_Flashbang.UI_Flashbang_C" true)))))
    (:CastFailed
      _))
  (return (LocalVariables|GetReceveid)))