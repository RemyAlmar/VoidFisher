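; BP_Pool is an object pool actor that reuses spawned actors of a configured class up to a size limit.
; LaunchPoolActor takes the last available actor, spawns a new one while under the limit, or recycles the first used one, then applies transform and string-keyed params.
; Pooled actors' come-to and back-to-pool events drive the Available and Used lists, with returned actors moved to the pool's location.
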(fn ConstructionScript
  (Default|AddParamsWithoutModify (Variables|Default|GetBPC_ParamsByString)))

(fn LaunchPoolActor
  (params (Transform :type Transform) (Params :type Map%20of%20Strings%20to%20Reals))
  (LocalVariables|SetTargetToSpawn (CallFunction|GetLastAvailable))
  (Utilities|IsValid (LocalVariables|GetTargetToSpawn)
    (:Is%20Valid
      (Transformation|SetActorTransform (LocalVariables|GetTargetToSpawn) Transform :!label _label)
      (Default|SetParams (Variables|/Game/Blueprints/AI/Spawnables/BP_PoolActor.BP_PoolActor_C|GetBPC_ParamsByString (LocalVariables|GetTargetToSpawn)) Params :!label _label_2)
      (Default|EDCometoPoolEvent (LocalVariables|GetTargetToSpawn))
      (return (LocalVariables|GetTargetToSpawn)))
    (:Is%20Not%20Valid
      (if (CallFunction|SizeMaxReached)
        (bind _output_get (LocalVariables|SetTargetToSpawn (CallFunction|GetFirstUsed)))
        (Default|EDBacktoPoolEvent _output_get)
        (Utilities|IsValid (LocalVariables|GetTargetToSpawn)
          (:Is%20Valid
            (goto _label))
          (:Is%20Not%20Valid
            (Development|PrintText "ERROR : Pool has not pool object used and can't spawn another" true true "(R=1.000000,G=0.000000,B=0.101372,A=1.000000)" 5e+01)))
        (else
          (LocalVariables|SetTargetToSpawn (CallFunction|SpawnPoolActorbyClass (Variables|Init|GetPoolClassActor) Transform))
          (EventDispatchers|BindEventtoEDBacktoPool (LocalVariables|GetTargetToSpawn) (EventDispatchers|CreateEvent :!event BacktoPool))
          (EventDispatchers|BindEventtoEDCometoPool (LocalVariables|GetTargetToSpawn) (EventDispatchers|CreateEvent :!event CometoPool))
          (goto _label_2))))))

(fn SpawnPoolActorbyClass
  (params (TargetClass :type BP%20Pool%20Actor%20Class%20Reference) (SpawnTransform :type Transform))
  (bind _returnvalue (Game|SpawnActorfromClass TargetClass SpawnTransform "AlwaysSpawn" "MultiplyWithRoot" 0 0))
  (return _returnvalue))

(fn CometoPool
  (params (TargetToAdd :type BP%20Pool%20Actor%20Object%20Reference%20%28by%20ref%29))
  (bind _available (Variables|HandlePool|GetAvailable))
  (if (Utilities|Array|ContainsItem _available TargetToAdd)
    (Utilities|Array|RemoveItem _available TargetToAdd))
  (Utilities|Array|AddUnique (Variables|HandlePool|GetUsed) TargetToAdd)
  (return))

(fn BacktoPool
  (params (TargetToAdd :type BP%20Pool%20Actor%20Object%20Reference%20%28by%20ref%29))
  (bind _used (Variables|HandlePool|GetUsed))
  (Transformation|SetActorLocation TargetToAdd (Transformation|GetActorLocation) false false)
  (if (Utilities|Array|ContainsItem _used TargetToAdd)
    (Utilities|Array|RemoveItem _used TargetToAdd))
  (Utilities|Array|AddUnique (Variables|HandlePool|GetAvailable) TargetToAdd)
  (return))

(fn GetCurrentNumberActors
  (return (+ (Utilities|Array|Length (Variables|HandlePool|GetAvailable)) (Utilities|Array|Length (Variables|HandlePool|GetUsed)))))

(fn SizeMaxReached
  (return (>= (CallFunction|GetCurrentNumberActors) (Variables|Init|GetPoolSize))))

(fn GetLastAvailable
  (bind _available (Variables|HandlePool|GetAvailable))
  (return (Utilities|Array|Get(acopy) _available (Utilities|Array|LastIndex _available))))

(fn GetFirstUsed
  (return (Utilities|Array|Get(acopy) (Variables|HandlePool|GetUsed))))