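; Onboarding bait fish actor that moves along a spline and triggers a one-time tutorial popup.
; A timeline drives the Sphere's position and rotation along the spline, using a FlipFlop to ping-pong between ends.
; On BeginPlay it builds a UI_BaseOneBoarding widget from a data table row.
; The construction script binds collision begin or end overlap to show that widget; closing it destroys the actor and hides the cursor.
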(event Custom|OnEndOverlap
  (params (OverlappedComponent :type Primitive%20Component%20Object%20Reference) (OtherActor :type Actor%20Object%20Reference) (OtherComp :type Primitive%20Component%20Object%20Reference) (OtherBodyIndex :type Integer))
  (if (Variables|Default|GetIsUseable)
    (Variables|Default|SetIsUseable false)
    (CallFunction|DisplayTutoWidget)))

(event Custom|OnBeginOverlap
  (params (OverlappedComponent :type Primitive%20Component%20Object%20Reference) (OtherActor :type Actor%20Object%20Reference) (OtherComp :type Primitive%20Component%20Object%20Reference) (OtherBodyIndex :type Integer) (bFromSweep :type Boolean) (SweepResult :type Hit%20Result%20Structure%20%28by%20ref%29))
  (if (Variables|Default|GetIsUseable)
    (Variables|Default|SetIsUseable false)
    (CallFunction|DisplayTutoWidget)))

(event Custom|DisplayTutoWidget
  (UserInterface|Viewport|AddtoViewport (Variables|Default|GetWidgetUsed) 0)
  (Default|CallEDonOpenMenu (Variables|Default|GetWidgetUsed))
  (Development|PrintText "Activation Tuto Event"))

(event Custom|Go%20To%20Spline
  (bind _spline (Variables|Default|GetSpline))
  (bind _sphere (Variables|Default|GetSphere))
  (Components|Timeline|SetPlayRate (Variables|Default|GetGoSpline) (Variables|Default|GetSpeed))
  (bind _length (Timeline|GoSpline PlayFromStart)
    (:Update
      (Transformation|SetWorldLocation _sphere (Spline|GetLocationatDistanceAlongSpline _spline (* _length (Spline|GetSplineLength _spline)) "World") false false)
      (Transformation|SetWorldRotation _sphere (Spline|GetRotationatDistanceAlongSpline _spline (* _length (Spline|GetSplineLength _spline)) "World") false false))
    (:Finished
      (Utilities|FlowControl|FlipFlop
        (:A
          (CallFunction|ReturntoSpline))
        (:B
          (CallFunction|GotoSpline))))))

(event Custom|ED_OnOpenWindow
  (Development|PrintText "Ouverture"))

(event Custom|ED_OnCloseWindow
  (Actor|DestroyActor)
  (Development|PrintText "Fermeture")
  (Variables|/Script/Engine.PlayerController|SetbShowMouseCursor (Game|GetPlayerController 0) false))

(event Custom|Return%20To%20Spline
  (bind _spline (Variables|Default|GetSpline))
  (bind _sphere (Variables|Default|GetSphere))
  (bind _length (Timeline|GoSpline ReverseFromEnd)
    (:Update
      (Transformation|SetWorldLocation _sphere (Spline|GetLocationatDistanceAlongSpline _spline (* _length (Spline|GetSplineLength _spline)) "World") false false)
      (Transformation|SetWorldRotation _sphere (Spline|GetRotationatDistanceAlongSpline _spline (* _length (Spline|GetSplineLength _spline)) "World") false false))
    (:Finished
      (Utilities|FlowControl|FlipFlop
        (:A
          (CallFunction|ReturntoSpline))
        (:B
          (CallFunction|GotoSpline))))))

(event EventBeginPlay
  (bind _returnvalue (UserInterface|CreateWidget "/Game/Blueprints/Widgets/OnBoarding/UI_BaseOneBoarding.UI_BaseOneBoarding_C" (Game|GetPlayerController 0) "/Game/SFX/Sounds/OGG/UI_UX/CUE/Fishopdeia/SFX_Menu_1_Cue.SFX_Menu_1_Cue" "/Game/SFX/Sounds/OGG/UI_UX/CUE/Fishopdeia/SFX_fermeture-01_Cue.SFX_fermeture-01_Cue" "/Game/SFX/Sounds/OGG/UI_UX/CUE/Fishopdeia/SFX_Menu_1_Cue.SFX_Menu_1_Cue"))
  (bind _output_get (Variables|Default|SetWidgetUsed _returnvalue))
  (Default|SetData _output_get (CallFunction|GetData))
  (EventDispatchers|BindEventtoEDonCloseMenu (Variables|Default|GetWidgetUsed) (EventDispatchers|CreateEvent :!event Custom|ED_OnCloseWindow))
  (EventDispatchers|BindEventtoEDonOpenMenu (Variables|Default|GetWidgetUsed) (EventDispatchers|CreateEvent :!event Custom|ED_OnOpenWindow))
  (CallFunction|GotoSpline))

(fn ConstructionScript
  (bind _shape_collision (Variables|Default|GetShape%20Collision))
  (if (Variables|Parameters|GetBeginOverlap)
    (Collision|BindEventtoOnComponentBeginOverlap _shape_collision (EventDispatchers|CreateEvent :!event Custom|OnBeginOverlap))
    (else
      (Collision|BindEventtoOnComponentEndOverlap _shape_collision (EventDispatchers|CreateEvent :!event Custom|OnEndOverlap)))))

(fn GetData
  (bind _data (Variables|Parameters|GetData))
  (bind _returnvalue (Utilities|GetDataTableRow (.datatable _data) (.rowname _data))
    (:then
      (return _returnvalue))))

(fn SetShape
  (switch Utilities|FlowControl|Switch|SwitchonE_CollisionShape (Variables|Parameters|Shape|GetShape)
    (:NewEnumerator1
      (Variables|Default|SetShape%20Collision 0))
    (:NewEnumerator0
      (Variables|Default|SetShape%20Collision 0))
    (:NewEnumerator2
      (Variables|Default|SetShape%20Collision 0)))
  (Collision|BindEventtoOnComponentEndOverlap (Variables|Default|GetShape%20Collision) (EventDispatchers|CreateEvent :!event Custom|OnEndOverlap))
  (Collision|BindEventtoOnComponentBeginOverlap (Variables|Default|GetShape%20Collision) (EventDispatchers|CreateEvent :!event Custom|OnBeginOverlap))
  (Rendering|SetVisibility (Variables|Default|GetShape%20Collision) true false)
  (Development|SetHiddeninGame (Variables|Default|GetShape%20Collision) (Variables|Parameters|GetHidden%20in%20Game) false))