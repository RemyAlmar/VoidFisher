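; BP_TutoCollider is a one-shot onboarding trigger that shows a tutorial widget when its sphere is overlapped.
; On BeginPlay it creates a UI_BaseOneBoarding widget, feeds it a configurable DataTable row and binds its open and close events.
; The construction script sets the sphere radius and uses a flag to trigger on begin or end overlap, without filtering actors.
; The first overlap opens the widget, and closing it destroys the actor.
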(event Custom|OnEndOverlap
  (params (OverlappedComponent :type Primitive%20Component%20Object%20Reference) (OtherActor :type Actor%20Object%20Reference) (OtherComp :type Primitive%20Component%20Object%20Reference) (OtherBodyIndex :type Integer))
  (if (Variables|Default|GetIsUseable)
    (Variables|Default|SetIsUseable false)
    (CallFunction|DisplayTutoWidget)))

(event Custom|OnBeginOverlap
  (params (OverlappedComponent :type Primitive%20Component%20Object%20Reference) (OtherActor :type Actor%20Object%20Reference) (OtherComp :type Primitive%20Component%20Object%20Reference) (OtherBodyIndex :type Integer) (bFromSweep :type Boolean) (SweepResult :type Hit%20Result%20Structure%20%28by%20ref%29))
  (if (Variables|Default|GetIsUseable)
    (Variables|Default|SetIsUseable false)
    (CallFunction|DisplayTutoWidget)))

(event Custom|DisplayTutoWidget
  (Default|EDonOpenMenuEvent (Variables|Default|GetWidgetUsed)))

(event Custom|ED_OnOpenWindow)

(event Custom|ED_OnCloseWindow
  (Actor|DestroyActor))

(event EventBeginPlay
  (bind _returnvalue (UserInterface|CreateWidget "/Game/Blueprints/Widgets/OnBoarding/UI_BaseOneBoarding.UI_BaseOneBoarding_C" (Game|GetPlayerController 0)))
  (bind _output_get (Variables|Default|SetWidgetUsed _returnvalue))
  (Default|SetGuide _output_get (CallFunction|GetData))
  (EventDispatchers|BindEventtoEDonCloseMenu (Variables|Default|GetWidgetUsed) (EventDispatchers|CreateEvent :!event Custom|ED_OnCloseWindow))
  (EventDispatchers|BindEventtoEDonOpenMenu (Variables|Default|GetWidgetUsed) (EventDispatchers|CreateEvent :!event Custom|ED_OnOpenWindow)))

(fn ConstructionScript
  (bind _sphere (Variables|Default|GetSphere))
  (Components|Sphere|SetSphereRadius (Variables|Default|GetSphere) (Variables|Parameters|GetRadius) true)
  (if (Variables|Parameters|GetBeginOverlap)
    (Collision|BindEventtoOnComponentBeginOverlap _sphere (EventDispatchers|CreateEvent :!event Custom|OnBeginOverlap))
    (else
      (Collision|BindEventtoOnComponentEndOverlap _sphere (EventDispatchers|CreateEvent :!event Custom|OnEndOverlap)))))

(fn GetData
  (bind _data (Variables|Parameters|GetData))
  (bind _returnvalue (Utilities|GetDataTableRow (.datatable _data) (.rowname _data))
    (:then
      (return _returnvalue))))