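; BP_TutosCollider is a one-shot onboarding trigger volume that fires when BP_PlayerRefonte overlaps it.
; If dialogue is enabled, it asks BP_TutoColliderManager, found on BeginPlay, to show the tutorial widget, with or without a timer depending on InputEvent.
; It then calls the linked Door to open and destroys itself.
; The construction script scales the box extent by BoxColliderSize.
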(event EventBeginPlay
  (bind _returnvalue (Actor|GetActorOfClass "/Game/Blueprints/Onboarding/BP_TutoColliderManager.BP_TutoColliderManager_C"))
  (Variables|Default|SetManager _returnvalue))

(event Collision|EventActorBeginOverlap
  (params (OtherActor :type Actor%20Object%20Reference))
  (bind _manager (Variables|Default|GetManager))
  (if (== (Utilities|GetClass OtherActor) "/Game/Blueprints/Game/Player/Controllers/BP_PlayerRefonte.BP_PlayerRefonte_C")
    (if (Variables|Default|GetIsUseable)
      (Variables|Default|SetIsUseable false)
      (if (Variables|Default|GetHave%20Dialogue)
        (if (Variables|Default|GetInputEvent)
          (Default|TutoWidget(NoTimer) _manager)
          (else
            (Default|TutoWidget(Timer) _manager))))
      (Default|CallEDOpenDoor (Variables|Parameters|GetDoor%20))
      (Actor|DestroyActor))))

(fn ConstructionScript
  (bind _box (Variables|Default|GetBox))
  (Components|Box|SetBoxExtent _box (* (Variables|Parameters|GetBox%20Collider%20Size) (Variables|/Script/Engine.BoxComponent|GetBoxExtent _box)) false))