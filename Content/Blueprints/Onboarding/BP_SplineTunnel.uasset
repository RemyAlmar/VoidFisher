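; BP_SplineTunnel is an onboarding actor that builds a tunnel by repeating a mesh along a spline.
; The construction script adds collision-enabled spline mesh components, spaced by the mesh's X bounds plus an offset, with count derived from spline length.
; Each segment takes its endpoints and tangents from distances along the spline, with tangent length clamped to the spacing to match segment size.
; The event graph has no active logic.
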(event EventBeginPlay)

(event Collision|EventActorBeginOverlap
  (params (OtherActor :type Actor%20Object%20Reference)))

(event EventTick
  (params (DeltaSeconds :type Float%20%28single-precision%29)))

(fn ConstructionScript
  (bind _output_get (Variables|Default|SetSpacing (CallFunction|GetSpacing)))
  (bind _output_get_2 (Variables|Default|SetNumber%20Of%20Instance (CallFunction|GetInstanceNumber _output_get)))
  (for _index (range 0 _output_get_2)
    (bind _returnvalue (AddComponent|AddSplineMeshComponent false))
    (Collision|SetCollisionEnabled _returnvalue "QueryAndPhysics")
    (SplineMesh|SetForwardAxis _returnvalue "X" true)
    (Components|StaticMesh|SetStaticMesh _returnvalue (Variables|Parameter|GetMesh))
    (SplineMesh|SetStartandEnd _returnvalue (CallFunction|Getlocationindex _index) (CallFunction|GetTangentIndex _index) (CallFunction|Getlocationindex (+ _index 1)) (CallFunction|GetTangentIndex (+ _index 1)) true :!class /Script/Engine.SplineMeshComponent)))

(fn GetSpacing
  (bind _mesh (Variables|Parameter|GetMesh))
  (bind _returnvalue (StaticMesh|GetBoundingBox _mesh))
  (bind (_min _max) (Utilities|Struct|BreakBox _returnvalue))
  (return (+ (.X (Math|Vector|BreakVector (- _max _min))) (Variables|Parameter|GetOffset))))

(fn Getlocationindex
  (params (ID :type Integer))
  (return (Spline|GetLocationatDistanceAlongSpline (Variables|Default|GetSpline) (* ID (Variables|Default|GetSpacing)) "Local")))

(fn GetTangentIndex
  (params (ID :type Integer))
  (return (Math|Vector|ClampVectorSize (Spline|GetTangentatDistanceAlongSpline (Variables|Default|GetSpline) (* ID (Variables|Default|GetSpacing)) "Local") 0.0 (Variables|Default|GetSpacing))))

(fn GetInstanceNumber
  (params (Spacing :type Float%20%28double-precision%29))
  (return (Math|Float|Floor (/ (Spline|GetSplineLength (Variables|Default|GetSpline)) Spacing))))