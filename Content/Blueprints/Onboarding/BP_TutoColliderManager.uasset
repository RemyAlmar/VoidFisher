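; Tutorial manager that shows onboarding dialogue from a data table in an on-screen widget.
; On BeginPlay it creates UI_BaseDialogueTuto for the first player, fills it with the table's first row using a timer and adds it to the screen.
; Timer and NoTimer TutoWidget events step an index through the cached row names, updating the same widget with or without a timer.
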(event Custom|Tuto%20Widget%20%28Timer%29
  (bind _result (Math|Integer|IncrementInt (Variables|Default|GetIndex))
    (:%20%20
      (bind _returnvalue (Utilities|GetDataTableRow (.datatable (Variables|Parameters|GetData)) (Utilities|Array|Get(acopy) (Variables|Default|GetOut%20Row%20Names) _result))
        (:then
          (Default|SetDatawithTimer (Variables|Default|GetWidgetUsed) _returnvalue))))))

(event Custom|Tuto%20Widget%20%28No%20timer%29
  (bind _result (Math|Integer|IncrementInt (Variables|Default|GetIndex))
    (:%20%20
      (bind _returnvalue (Utilities|GetDataTableRow (.datatable (Variables|Parameters|GetData)) (Utilities|Array|Get(acopy) (Variables|Default|GetOut%20Row%20Names) _result))
        (:then
          (Default|SetDataWithoutTimer (Variables|Default|GetWidgetUsed) _returnvalue))))))

(event EventBeginPlay
  (bind _returnvalue (UserInterface|CreateWidget "/Game/Blueprints/Widgets/OnBoarding/UI_BaseDialogueTuto.UI_BaseDialogueTuto_C" (Game|GetPlayerController 0) "/Game/SFX/Sounds/OGG/UI_UX/CUE/Menu/SFX_Menu_1_Cue.SFX_Menu_1_Cue"))
  (bind _output_get (Variables|Default|SetWidgetUsed _returnvalue))
  (Default|SetDatawithTimer _output_get (CallFunction|GetData))
  (Default|CallEDonOpenMenu (Variables|Default|GetWidgetUsed))
  (UserInterface|Viewport|AddtoPlayerScreen (Variables|Default|GetWidgetUsed)))

(fn ConstructionScript)

(fn GetData
  (bind _data (Variables|Parameters|GetData))
  (bind _outrownames (DataTable|GetDataTableRowNames (.datatable _data)))
  (bind _output_get (Variables|Default|SetOut%20Row%20Names _outrownames))
  (bind _returnvalue (Utilities|GetDataTableRow (.datatable _data) (Utilities|Array|Get(acopy) _output_get))
    (:then
      (return _returnvalue))))