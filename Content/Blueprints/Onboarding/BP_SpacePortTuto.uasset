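; Onboarding space port trigger that opens a ship HUD menu and pauses the game when the player enters its box.
; On overlap it casts to BP_PlayerRefonte, clears the other HUD menus, toggles the target widget and pauses.
; ActiveOverlap switches the box's overlap events on or off and fires the matching open or close event dispatcher.
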(event OnComponentBeginOverlap(Box)
  (params (OverlappedComponent :type Primitive%20Component%20Object%20Reference) (OtherActor :type Actor%20Object%20Reference) (OtherComp :type Primitive%20Component%20Object%20Reference) (OtherBodyIndex :type Integer) (bFromSweep :type Boolean) (SweepResult :type Hit%20Result%20Structure%20%28by%20ref%29))
  (bind _asbp_player_refonte (Utilities|Casting|CastToBP_PlayerRefonte OtherActor))
  (bind _output_get (Variables|Default|SetPlayerRefonte _asbp_player_refonte))
  (Default|ClearAllExceptMenuTarget (Variables|/Game/Blueprints/Game/Player/Controllers/BP_PlayerRefonte.BP_PlayerRefonte_C|GetHUD_Ship _output_get) "NewEnumerator23")
  (Default|ToggleWidget (Variables|/Game/Blueprints/Game/Player/Controllers/BP_PlayerRefonte.BP_PlayerRefonte_C|GetHUD_Ship _output_get) "NewEnumerator23")
  (Game|SetGamePaused true))

(fn ConstructionScript)

(fn ActiveOverlap
  (params (Active :type Boolean))
  (bind _output_get (Variables|/Script/Engine.PrimitiveComponent|SetbGenerateOverlapEvents (Variables|Default|GetBox) Active))
  (if _output_get
    (Default|CallEDonOpen)
    (else
      (Default|CallEDonClose))))