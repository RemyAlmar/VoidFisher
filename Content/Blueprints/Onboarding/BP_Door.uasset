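; Two-panel sliding door in the onboarding content that opens on an event dispatcher and closes when the player enters its collision.
; BeginPlay binds to the open dispatcher and caches both panels' starting relative locations; EdOpenDoor runs a timeline moving them apart vertically.
; A BP_PlayerRefonte overlap with OpenCollision stops that timeline, then after a short delay runs a closing timeline back to the cached positions.
; Both timelines use configurable play rates and lerp from current locations.
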(event OnComponentBeginOverlap(OpenCollision)
  (params (OverlappedComponent :type Primitive%20Component%20Object%20Reference) (OtherActor :type Actor%20Object%20Reference) (OtherComp :type Primitive%20Component%20Object%20Reference) (OtherBodyIndex :type Integer) (bFromSweep :type Boolean) (SweepResult :type Hit%20Result%20Structure%20%28by%20ref%29))
  (bind _door1 (Variables|Default|GetDoor1))
  (bind _door (Variables|Default|GetDoor))
  (bind _relativelocation (Variables|/Script/Engine.SceneComponent|GetRelativeLocation _door))
  (bind _relativelocation_2 (Variables|/Script/Engine.SceneComponent|GetRelativeLocation _door1))
  (if (== (Utilities|GetClass OtherActor) "/Game/Blueprints/Game/Player/Controllers/BP_PlayerRefonte.BP_PlayerRefonte_C")
    (Utilities|FlowControl|Sequence
      (:then_0
        (bind _open (Timeline|DoorMovementOpen Stop)
          (:Update
            (Transformation|SetRelativeLocation _door (Math|Vector|Lerp(Vector) _relativelocation "0.000000,0.000000,30000.000000" _open) false false)
            (Transformation|SetRelativeLocation (Variables|Default|GetDoor1) (Math|Vector|Lerp(Vector) _relativelocation_2 "0.000000,0.000000,-30000.000000" _open) false false))))
      (:then_1
        (Utilities|FlowControl|Delay 0.5)
        (Components|Timeline|SetPlayRate (Variables|Default|GetDoorMovementClose) (Variables|Parameter|GetClose%20Door%20Speed))
        (bind _close (Timeline|DoorMovementClose Play)
          (:Update
            (Transformation|SetRelativeLocation _door (Math|Vector|Lerp(Vector) _relativelocation (Variables|Default|GetDoor%20du%20haut) _close) false false)
            (Transformation|SetRelativeLocation (Variables|Default|GetDoor1) (Math|Vector|Lerp(Vector) _relativelocation_2 (Variables|Default|GetDoor%20du%20bas) _close) false false)))))))

(event Custom|Ed%20Open%20Door
  (bind _door (Variables|Default|GetDoor))
  (Components|Timeline|SetPlayRate (Variables|Default|GetDoorMovementOpen) (Variables|Parameter|GetOpen%20Door%20speed))
  (bind _open (Timeline|DoorMovementOpen Play)
    (:Update
      (Transformation|SetRelativeLocation _door (Math|Vector|Lerp(Vector) (Variables|/Script/Engine.SceneComponent|GetRelativeLocation _door) "0.000000,0.000000,30000.000000" _open) false false)
      (Transformation|SetRelativeLocation (Variables|Default|GetDoor1) (Math|Vector|Lerp(Vector) (Variables|/Script/Engine.SceneComponent|GetRelativeLocation (Variables|Default|GetDoor1)) "0.000000,0.000000,-30000.000000" _open) false false))))

(event EventBeginPlay
  (EventDispatchers|BindEventtoEDOpenDoor (EventDispatchers|CreateEvent :!event Custom|Ed%20Open%20Door))
  (Variables|Default|SetDoor%20du%20haut (Variables|/Script/Engine.SceneComponent|GetRelativeLocation (Variables|Default|GetDoor)))
  (Variables|Default|SetDoor%20du%20bas (Variables|/Script/Engine.SceneComponent|GetRelativeLocation (Variables|Default|GetDoor1))))

(event EventTick
  (params (DeltaSeconds :type Float%20%28single-precision%29)))

(fn ConstructionScript)