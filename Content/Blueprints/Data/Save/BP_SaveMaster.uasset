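; BP_SaveMaster keeps the list of save slot names for the game's save data.
; Adding a slot removes any existing entry and appends it at the end, so the list stays ordered by most recent addition and GetLastSlot returns the newest name.
; It also removes slots, reports whether any save exists, and prints every slot with its index.
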(fn AddSlotSave
  (params (TargetName :type String))
  (bind _saveslotnamelist (Variables|Default|GetSaveSlotNameList))
  (if (Utilities|Array|ContainsItem _saveslotnamelist TargetName)
    (Utilities|Array|RemoveItem _saveslotnamelist TargetName))
  (Utilities|Array|AddUnique (Variables|Default|GetSaveSlotNameList) TargetName)
  (return))

(fn RemoveSlotSave
  (params (ItemToFind :type String%20%28by%20ref%29))
  (bind _saveslotnamelist (Variables|Default|GetSaveSlotNameList))
  (if (Utilities|Array|ContainsItem _saveslotnamelist ItemToFind)
    (Utilities|Array|RemoveItem _saveslotnamelist ItemToFind)
    (return)))

(fn GetLastSlot
  (bind _saveslotnamelist (Variables|Default|GetSaveSlotNameList))
  (if (CallFunction|HasASave)
    (LocalVariables|SetSaveSlotName (Utilities|Array|Get(acopy) _saveslotnamelist (Utilities|Array|LastIndex _saveslotnamelist)))
    (return (LocalVariables|GetSaveSlotName))))

(fn HasASave
  (return (Utilities|Array|IsNotEmpty (Variables|Default|GetSaveSlotNameList))))

(fn DisplayAllSlotSave
  (for (_array_element _array_index) (Variables|Default|GetSaveSlotNameList)
    (Development|PrintText 0 (Utilities|Text|FormatText "{x} {y}" (Utilities|String|Append (Utilities|String|Append "Save_" (Utilities|String|ToString(Integer) _array_index)) "_") _array_element) true true "(R=1.000000,G=0.271328,B=0.000000,A=1.000000)" 0.0)))