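; Save slot data for VoidFisher, holding a slot name, save timestamp and the active state of parasite actors across the world.
; Parasite states live in nested maps keyed by area, micro area, then actor name.
; Setters write back up through each map level and fire a parasite-activity dispatcher, while getters add missing keys on lookup.
; Helpers count total, active and inactive parasites per area or micro area and print states for debugging.
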(fn SetMapParasitebyArea
  (params (Key :type Byte) (Value :type S%20Array%20Map%20Actor%20Bool%20Structure%20%28by%20ref%29))
  (bind _output_get (LocalVariables|SetCurrentMicroAreas (Variables|Scenes|Parasite|GetS_ParasiteActif)))
  (Utilities|Map|Add (.arraymap _output_get) Key Value)
  (|SetBy-RefVar (Variables|Scenes|Parasite|GetS_ParasiteActif) (LocalVariables|GetCurrentMicroAreas))
  (Default|CallEDonSetParasiteActivity)
  (return))

(fn SetParasiteActivity
  (params (Area :type Byte) (MicroArea :type Byte%20%28by%20ref%29) (TargetName :type String%20%28by%20ref%29) (IsActif :type Boolean))
  (bind _output_get (LocalVariables|SetCurrentMicroStruct (.Value (Scenes|Parasite|GetMapParasitebyMicroArea Area MicroArea))))
  (Utilities|Map|Add (.actorissomething _output_get) TargetName IsActif)
  (Scenes|Parasite|SetMapParasitebyMicroArea Area MicroArea (LocalVariables|GetCurrentMicroStruct)))

(fn GetMapParasitebyArea
  (params (Key :type Byte))
  (bind _s_parasiteactif (Variables|Scenes|Parasite|GetS_ParasiteActif))
  (bind (_value _returnvalue) (Utilities|Map|Find (.arraymap _s_parasiteactif) Key))
  (if _returnvalue
    _
    (else
      (Utilities|Map|Add :TargetMap (.arraymap _s_parasiteactif) :Key Key)))
  (return _value _returnvalue))

(fn GetParasiteNumberbyArea
  (params (Area :type Byte))
  (bind _value (Scenes|Parasite|GetMapParasitebyArea Area))
  (bind _activenumber (LocalVariables|GetActiveNumber))
  (bind _keys (Utilities|Map|Keys (.mapenumactorbool _value)))
  (LocalVariables|SetTotalActors (CallFunction|GetNumberNamebyArea Area))
  (for _array_element _keys
    (bind _values (Utilities|Map|Values (.actorissomething (.Value (Utilities|Map|Find (.mapenumactorbool _value) _array_element)))))
    (for _array_element_2 _values
      (if _array_element_2
        (Math|Integer|IncrementInt (LocalVariables|GetActiveNumber)))))
  (return (LocalVariables|GetTotalActors) _activenumber (- (LocalVariables|GetTotalActors) _activenumber)))

(fn SetCurrentSaveDateTime
  (Variables|Default|SetCurrentDateTime (Math|DateTime|Now))
  (return))

(fn SetSlotName
  (params (SlotName :type String))
  (bind _output_get (Variables|Slot|SetSlotName SlotName))
  (if (Utilities|Array|IsEmpty _output_get)
    (Variables|Slot|SetSlotName (Utilities|String|Replace (Utilities|String|Append "VoidFisher_" (Utilities|String|ToString(Text) (Class|KismetTextLibrary|AsTimeDateTime (Math|DateTime|Now)))) ":" "_")))
  (return))

(fn ActorIsActive
  (params (TargetName :type String%20%28by%20ref%29) (Area :type Byte) (MicroArea :type Byte%20%28by%20ref%29))
  (bind _value (Scenes|Parasite|GetMapParasitebyMicroArea Area MicroArea))
  (bind (_value_2 _returnvalue) (Utilities|Map|Find (.actorissomething _value) TargetName))
  (return _returnvalue _value_2))

(fn GetNumberNamebyArea
  (params (Area :type Byte))
  (bind _s_parasiteactif (Variables|Scenes|Parasite|GetS_ParasiteActif))
  (bind _value (Utilities|Map|Find (.arraymap _s_parasiteactif) Area))
  (bind _keys (Utilities|Map|Keys (.mapenumactorbool _value)))
  (for _array_element _keys
    (LocalVariables|SetTotalActors (+ (LocalVariables|GetTotalActors) (Utilities|Map|Length (.actorissomething (.Value (Utilities|Map|Find (.mapenumactorbool _value) _array_element)))))))
  (return (LocalVariables|GetTotalActors)))

(fn DisplayActorsActivitiesbyArea
  (params (Area :type Byte))
  (bind _values (Utilities|Map|Values (.mapenumactorbool (.Value (Utilities|Map|Find (.arraymap (Variables|Scenes|Parasite|GetS_ParasiteActif)) Area)))))
  (for _array_element _values
    (bind _output_get (LocalVariables|SetCurrentActorsActiivities (.actorissomething _array_element)))
    (bind _keys (Utilities|Map|Keys _output_get))
    (for _array_element_2 _keys
      (Development|PrintText 0 (Utilities|Text|FormatText "Actor : {x} / Is Active : {y}" _array_element_2 (.Value (Utilities|Map|Find (LocalVariables|GetCurrentActorsActiivities) _array_element_2))) true true "(R=0.125281,G=1.000000,B=0.100480,A=1.000000)" 0.0))))

(fn GetMapParasitebyMicroArea
  (params (Area :type Byte) (MicroArea :type Byte%20%28by%20ref%29))
  (bind _value (Scenes|Parasite|GetMapParasitebyArea Area))
  (bind (_value_2 _returnvalue) (Utilities|Map|Find (.mapenumactorbool _value) MicroArea))
  (Utilities|Map|Add (.mapenumactorbool _value) MicroArea _value_2)
  (return _value_2 _returnvalue))

(fn GetParasiteNumberbyMicroArea
  (params (Area :type Byte) (MicroArea :type Byte%20%28by%20ref%29))
  (bind _activenumber (LocalVariables|GetActiveNumber))
  (LocalVariables|SetTotalActors (CallFunction|GetNumberNamebyMicroArea Area MicroArea))
  (bind _values (Utilities|Map|Values (.actorissomething (.Value (Scenes|Parasite|GetMapParasitebyMicroArea Area MicroArea)))))
  (for _array_element _values
    (if _array_element
      (Math|Integer|IncrementInt (LocalVariables|GetActiveNumber))))
  (return (LocalVariables|GetTotalActors) _activenumber (- (LocalVariables|GetTotalActors) _activenumber)))

(fn GetNumberNamebyMicroArea
  (params (Area :type Byte) (MicroArea :type Byte%20%28by%20ref%29))
  (return (Utilities|Map|Length (.actorissomething (.Value (Utilities|Map|Find (.mapenumactorbool (.Value (Utilities|Map|Find (.arraymap (Variables|Scenes|Parasite|GetS_ParasiteActif)) Area))) MicroArea))))))

(fn SetMapParasitebyMicroArea
  (params (Area :type Byte) (MicroArea :type Byte) (Value :type S%20Map%20Actor%20Bool%20Structure%20%28by%20ref%29))
  (bind _output_get (LocalVariables|SetCurrentArea (.Value (Scenes|Parasite|GetMapParasitebyArea Area))))
  (Utilities|Map|Add (.mapenumactorbool _output_get) MicroArea Value)
  (Scenes|Parasite|SetMapParasitebyArea Area (LocalVariables|GetCurrentArea))
  (return))