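; Global data component for the fishing game that serves Fishopedia data and tracks the player's catches.
; On BeginPlay it seeds per-species dictionaries for record weight and bag count from every DT_Fishopedia row name.
; Tag-based getters read name, lore, image, spawn zone and weight range from the table, which also feeds random weight rolls.
; Setters keep the heaviest weight and increment counts, and a query totals all fish caught.
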(event EventBeginPlay
  ;[0 0 0] instance DATA
  (bind _output_get (Variables|Default|SetDT_Fishopedia "/Game/Blueprints/Data/DT_Fishopedia.DT_Fishopedia"))
  (bind _outrownames (DataTable|GetDataTableRowNames _output_get))
  (for _index (range 0 (Utilities|Array|LastIndex _outrownames))
    (Utilities|FlowControl|Sequence
      (:then_0
        (Utilities|Map|Add (Variables|Default|GetDct_Weight) (Utilities|Array|Get(acopy) _outrownames _index) 0.0)
        (Variables|Default|SetF_TotalFish 0))
      (:then_1
        (Utilities|Map|Add (Variables|Default|GetDct_FishInBag) (Utilities|Array|Get(acopy) _outrownames _index) 0)))))

(fn GetNameValue
  (params (Tag :type Name :default "TinyFish1"))
  (bind _dt_fishopedia (Variables|Default|GetDT_Fishopedia))
  (bind _returnvalue (Class|DataTableFunctionLibrary|DoesDataTableRowExist _dt_fishopedia Tag))
  (if _returnvalue
    (bind _returnvalue_2 (Utilities|GetDataTableRow _dt_fishopedia Tag)
      (:then
        _)
      (:RowNotFound
        (Development|PrintString "Row not found" true true "(R=1.000000,G=0.683303,B=0.000000,A=1.000000)" :!label _label)))
    (else
      (Development|PrintString "Tag not in data base" true true "(R=1.000000,G=0.022033,B=0.000000,A=1.000000)")
      (goto _label)))
  (return (.FishName (Utilities|Struct|BreakBS_Fishopedia _returnvalue_2))))

(fn GetAllData
  (params (Tag :type Name))
  (bind _dt_fishopedia (Variables|Default|GetDT_Fishopedia))
  (bind _returnvalue (Class|DataTableFunctionLibrary|DoesDataTableRowExist _dt_fishopedia Tag))
  (if _returnvalue
    (bind _returnvalue_2 (Utilities|GetDataTableRow _dt_fishopedia Tag)
      (:then
        _)
      (:RowNotFound
        (Development|PrintString "Row not found" true true "(R=1.000000,G=0.683303,B=0.000000,A=1.000000)" :!label _label)))
    (else
      (Development|PrintString "Tag not in data base" true true "(R=1.000000,G=0.022033,B=0.000000,A=1.000000)")
      (goto _label)))
  (return (.FishName (Utilities|Struct|BreakBS_Fishopedia _returnvalue_2)) (.Lore (Utilities|Struct|BreakBS_Fishopedia _returnvalue_2)) (.Image (Utilities|Struct|BreakBS_Fishopedia _returnvalue_2)) (.ZoneSpawn (Utilities|Struct|BreakBS_Fishopedia _returnvalue_2)) (.WeightMaxkg (Utilities|Struct|BreakBS_Fishopedia _returnvalue_2)) (.WeightMinkg (Utilities|Struct|BreakBS_Fishopedia _returnvalue_2))))

(fn GetLoreValue
  (params (Tag :type Name))
  (bind _dt_fishopedia (Variables|Default|GetDT_Fishopedia))
  (bind _returnvalue (Class|DataTableFunctionLibrary|DoesDataTableRowExist _dt_fishopedia Tag))
  (if _returnvalue
    (bind _returnvalue_2 (Utilities|GetDataTableRow _dt_fishopedia Tag)
      (:then
        _)
      (:RowNotFound
        (Development|PrintString "Row not found" true true "(R=1.000000,G=0.683303,B=0.000000,A=1.000000)" :!label _label)))
    (else
      (Development|PrintString "Tag not in data base" true true "(R=1.000000,G=0.022033,B=0.000000,A=1.000000)")
      (goto _label)))
  (return (.Lore (Utilities|Struct|BreakBS_Fishopedia _returnvalue_2))))

(fn GetImageValue
  (params (Tag :type Name))
  (bind _dt_fishopedia (Variables|Default|GetDT_Fishopedia))
  (bind _returnvalue (Class|DataTableFunctionLibrary|DoesDataTableRowExist _dt_fishopedia Tag))
  (if _returnvalue
    (bind _returnvalue_2 (Utilities|GetDataTableRow _dt_fishopedia Tag)
      (:then
        _)
      (:RowNotFound
        (Development|PrintString "Row not found" true true "(R=1.000000,G=0.683303,B=0.000000,A=1.000000)" :!label _label)))
    (else
      (Development|PrintString "Tag not in data base" true true "(R=1.000000,G=0.022033,B=0.000000,A=1.000000)")
      (goto _label)))
  (return (.Image (Utilities|Struct|BreakBS_Fishopedia _returnvalue_2))))

(fn GetZoneSpawnValue
  (params (Tag :type Name))
  (bind _dt_fishopedia (Variables|Default|GetDT_Fishopedia))
  (bind _returnvalue (Class|DataTableFunctionLibrary|DoesDataTableRowExist _dt_fishopedia Tag))
  (if _returnvalue
    (bind _returnvalue_2 (Utilities|GetDataTableRow _dt_fishopedia Tag)
      (:then
        _)
      (:RowNotFound
        (Development|PrintString "Row not found" true true "(R=1.000000,G=0.683303,B=0.000000,A=1.000000)" :!label _label)))
    (else
      (Development|PrintString "Tag not in data base" true true "(R=1.000000,G=0.022033,B=0.000000,A=1.000000)")
      (goto _label)))
  (return (.ZoneSpawn (Utilities|Struct|BreakBS_Fishopedia _returnvalue_2))))

(fn GetMaxandMinWeight
  (params (Tag :type Name))
  (bind _dt_fishopedia (Variables|Default|GetDT_Fishopedia))
  (bind _returnvalue (Class|DataTableFunctionLibrary|DoesDataTableRowExist _dt_fishopedia Tag))
  (if _returnvalue
    (bind _returnvalue_2 (Utilities|GetDataTableRow _dt_fishopedia Tag)
      (:then
        _)
      (:RowNotFound
        (Development|PrintString "Row not found" true true "(R=1.000000,G=0.683303,B=0.000000,A=1.000000)" :!label _label)))
    (else
      (Development|PrintString "Tag not in data base" true true "(R=1.000000,G=0.022033,B=0.000000,A=1.000000)")
      (goto _label)))
  (return (.WeightMaxkg (Utilities|Struct|BreakBS_Fishopedia _returnvalue_2)) (.WeightMinkg (Utilities|Struct|BreakBS_Fishopedia _returnvalue_2))))

(fn ReturnTotalFishCaught
  (Variables|Default|SetF_TotalFish 0)
  (bind _values (Utilities|Map|Values (Variables|Default|GetDct_FishInBag)))
  (for _array_element _values
    (bind _output_get (Variables|Default|SetF_TotalFish (+ _array_element (Variables|Default|GetF_TotalFish)))))
  (return _output_get))

(fn GetFishCoughtbyName
  (params (Tag :type Name%20%28by%20ref%29))
  (bind _dct_fishinbag (Variables|Default|GetDct_FishInBag))
  (bind (_value _returnvalue) (Utilities|Map|Find _dct_fishinbag Tag))
  (if _returnvalue
    _
    (else
      (Development|PrintString "Tag is not in row")))
  (return _value))

(fn RandomWeight
  (params (Tag :type Name))
  (bind (_weight_max__kg_ _weight_min__kg_) (Get|GetMaxandMinWeight Tag))
  (return (Math|Random|RandomFloatinRange _weight_min__kg_ _weight_max__kg_)))

(fn SetNewWeight
  (params (Tag :type Name%20%28by%20ref%29) (Weight :type Float%20%28double-precision%29))
  (bind _dct_weight (Variables|Default|GetDct_Weight))
  (bind (_value _returnvalue) (Utilities|Map|Find _dct_weight Tag))
  (if (and (> Weight _value) _returnvalue)
    (Utilities|Map|Add _dct_weight Tag Weight)
    (else
      (Development|PrintString "Tag is not valid")))
  (return))

(fn SetNewFishinBag
  (params (Key :type Name%20%28by%20ref%29))
  (bind _dct_fishinbag (Variables|Default|GetDct_FishInBag))
  (bind (_value _returnvalue) (Utilities|Map|Find _dct_fishinbag Key))
  (if _returnvalue
    (Utilities|Map|Add _dct_fishinbag Key (+ _value 1))
    (else
      (Development|PrintString "Tag is not valid")))
  (return))