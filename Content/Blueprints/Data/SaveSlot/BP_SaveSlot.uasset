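; Save slot data Blueprint that tracks which parasites are active in each area.
; A nested map in SParasiteActif links each area key to a map of actors and their active flags.
; SetParasiteActivity updates one actor's flag, then passes that area's map to SetMapParasiteByArea, which fires the OnSetParasiteActivity dispatcher.
; Getters return an area's map or its total, active and inactive parasite counts.
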(fn SetMapParasitebyArea
  (params (Key :type Byte%20%28by%20ref%29) (Value :type Map%20of%20Actor%20Object%20References%20to%20Booleans))
  (|SetBy-RefVar (.actorissomething (.Value (Utilities|Map|Find (.mapenumactorbool (Variables|Scenes|Parasite|GetS_ParasiteActif)) Key))) Value)
  (Default|CallEDonSetParasiteActivity)
  (return))

(fn SetParasiteActivity
  (params (Key :type Byte) (Target :type Actor%20Object%20Reference%20%28by%20ref%29) (IsActif :type Boolean))
  (bind _s_parasiteactif (Variables|Scenes|Parasite|GetS_ParasiteActif))
  (bind _value (Utilities|Map|Find (.mapenumactorbool _s_parasiteactif) Key))
  (Utilities|Map|Add (.actorissomething _value) Target IsActif)
  (Scenes|Parasite|SetMapParasitebyArea Key (.actorissomething _value)))

(fn GetMapParasitebyArea
  (params (Key :type Byte))
  (return (.actorissomething (.Value (Utilities|Map|Find (.mapenumactorbool (Variables|Scenes|Parasite|GetS_ParasiteActif)) Key)))))

(fn GetParasiteNumberbyArea
  (params (Key :type Byte%20%28by%20ref%29))
  (bind _s_parasiteactif (Variables|Scenes|Parasite|GetS_ParasiteActif))
  (bind _activenumber (LocalVariables|GetActiveNumber))
  (bind _value (Utilities|Map|Find (.mapenumactorbool _s_parasiteactif) Key))
  (bind _returnvalue (Utilities|Map|Length (.actorissomething _value)))
  (bind _values (Utilities|Map|Values (.actorissomething (.Value (Utilities|Map|Find (.mapenumactorbool (Variables|Scenes|Parasite|GetS_ParasiteActif)) Key)))))
  (for _array_element _values
    (if _array_element
      (Math|Integer|IncrementInt (LocalVariables|GetActiveNumber))))
  (return _returnvalue _activenumber (- _returnvalue _activenumber)))