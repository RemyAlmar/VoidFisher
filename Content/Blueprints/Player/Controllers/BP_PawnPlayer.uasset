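; Player vehicle pawn with throttle-driven forward movement, tuned through BaseVehicleOptions.
; MoveForward and MoveBack ramp a throttle timer up or down, scale it linearly to throttle, then add input times throttle to a clamped speed.
; Tick applies that speed along the actor's forward vector as FloatingPawnMovement velocity and prints debug readouts.
; Rotation switching, vertical and horizontal movement, and the delayed post-acceleration decrease are print-only stubs.
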(event EventMoveForward
  (params (Value :type Float%20%28double-precision%29))
  (CallFunction|HandleThrottleIncrease Value)
  (CallFunction|ApplyForwardMovement Value)
  (Utilities|FlowControl|RetriggerableDelay 1.0)
  (Development|PrintString "Start to decrease"))

(event EventMoveBack
  (params (Value :type Float%20%28double-precision%29))
  (CallFunction|HandleThrottleDecrease Value)
  (CallFunction|ApplyForwardMovement Value))

(event EventVerticalMovement
  (params (AxisValue :type Float%20%28double-precision%29))
  (Development|PrintString "Vertical"))

(event EventSwitchRotationMode
  (params (boolvalue :type Boolean))
  (Development|PrintString "Switch"))

(event EventHorizontalMovement
  (params (AxisValue :type Float%20%28double-precision%29))
  (Development|PrintString "Horizontal"))

(event EventTick
  (params (DeltaSeconds :type Float%20%28single-precision%29))
  (bind _basevehicleoptions (Variables|StructureVehiculeOptions|GetBaseVehicleOptions))
  (Variables|Default|SetDeltaTime DeltaSeconds)
  (Variables|/Script/Engine.MovementComponent|SetVelocity (Variables|Default|GetFloatingPawnMovement) (CallFunction|ThrottleForward (Variables|VehicleParametres|GetCurrentSpeed)))
  (Development|PrintText (Utilities|Text|FormatText "Vitesse : {speed} / {speedMax}" (Variables|VehicleParametres|GetCurrentSpeed) (.speedmax _basevehicleoptions)) true true "(R=1.000000,G=0.000000,B=0.199603,A=1.000000)" 0.0)
  (Development|PrintText (Utilities|Text|FormatText "Accel : {speed} / {speedMax}" (Variables|VehicleParametres|GetCurrentThrottle) (.throttlemax _basevehicleoptions)) true true "(R=0.041610,G=1.000000,B=0.990053,A=1.000000)" 0.0))

(fn ConstructionScript)

(fn ApplyForwardMovement
  (params (Value :type Float%20%28double-precision%29))
  (Variables|VehicleParametres|SetCurrentSpeed (Math|Float|Clamp(Float) (+ (Variables|VehicleParametres|GetCurrentSpeed) (* Value (Variables|VehicleParametres|GetCurrentThrottle))) 0.0 (.SpeedMax (Utilities|Struct|BreakStruct_VehicleOptions (Variables|StructureVehiculeOptions|GetBaseVehicleOptions)))))
  (return))

(fn ThrottleForward
  (params (Value :type Float%20%28double-precision%29))
  (return (* Value (Transformation|GetActorForwardVector))))

(fn HandleThrottleIncrease
  (params (SpeedToIncrease :type Float%20%28double-precision%29))
  (bind _basevehicleoptions (Variables|StructureVehiculeOptions|GetBaseVehicleOptions))
  (bind (_speedmax _brake _maniability _throttlemax _throttletimemax) (Utilities|Struct|BreakStruct_VehicleOptions _basevehicleoptions))
  (if (CallFunction|TimerPos (Variables|VehicleParametres|GetCurrentThrottleTime) _throttletimemax (* (Variables|Default|GetDeltaTime) SpeedToIncrease))
    (Variables|VehicleParametres|SetCurrentThrottleTime _throttletimemax))
  (Variables|VehicleParametres|SetCurrentThrottle (* _throttlemax (Math|Float|NormalizetoRange (Math|Float|Lerp 0.0 _throttletimemax (/ (Variables|VehicleParametres|GetCurrentThrottleTime) _throttletimemax)) 0.0 _throttletimemax))))

(fn HandleThrottleDecrease
  (params (SpeedToIncrease :type Float%20%28double-precision%29))
  (bind _basevehicleoptions (Variables|StructureVehiculeOptions|GetBaseVehicleOptions))
  (bind (_speedmax _brake _maniability _throttlemax _throttletimemax) (Utilities|Struct|BreakStruct_VehicleOptions _basevehicleoptions))
  (if (CallFunction|TimerNeg (Variables|VehicleParametres|GetCurrentThrottleTime) (* (Variables|Default|GetDeltaTime) SpeedToIncrease) 0.0)
    _
    (else
      _))
  (Variables|VehicleParametres|SetCurrentThrottle (* _throttlemax (Math|Float|NormalizetoRange (Math|Float|Lerp 0.0 _throttletimemax (/ (Variables|VehicleParametres|GetCurrentThrottleTime) _throttletimemax)) 0.0 _throttletimemax))))