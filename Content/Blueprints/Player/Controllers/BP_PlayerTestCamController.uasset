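; Test player spaceship Blueprint that flies a physics-driven ship with look steering, manual roll and forward/back throttle.
; Throttle events ease SpeedShip, which Tick decays, prints and uses as an exponent on rotation speed.
; Tick lerps PointReferenceMesh's velocity along actor forward, scaled by speed and a ShipStop factor that fades near standstill.
; RollShip cosmetically tilts SPAShip from look input, inverting pitch when not moving forward and easing back when idle.
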(event EventHorizontalRoll
  (params (AxisValue :type Float%20%28double-precision%29))
  ;[0.4203 0.3757 1] Roll Ship
  (Transformation|AddActorLocalRotation (Math|Rotator|MakeRotator (* AxisValue (Variables|Default|GetRollPlayerSpeed)) 0.0 0.0) false false))

(event EventTick
  (params (DeltaSeconds :type Float%20%28single-precision%29))
  ;[0.9969 1 0.5568] Move Forward
  (Utilities|FlowControl|Sequence
    (:then_0
      (CallFunction|MoveShipbySpeed))
    (:then_1
      (CallFunction|RollShip DeltaSeconds (.x (stale EventCameraLook LookDirection)) (.y (stale EventCameraLook LookDirection))))
    (:then_2
      (if (and (>= (Variables|Speed|GetSpeedShip) -0.1) (<= (Variables|Speed|GetSpeedShip) 0.1))
        (Variables|Speed|SetShipStop (Math|Interpolation|FInterpTo (Variables|Speed|GetShipStop) 0.0 0.5 1.0))
        (else
          (Variables|Speed|SetShipStop (Math|Interpolation|FInterpTo (Variables|Speed|GetShipStop) 1.0 0.5 1.0)))))
    (:then_3
      (Variables|Speed|SetSpeedShip (Math|Interpolation|FInterpTo (Variables|Speed|GetSpeedShip) 0.0 DeltaSeconds 0.05))
      (Variables|Default|SetCurrent%20Rotation%20Speed (* (Math|Float|Sign(Float) (Variables|Default|GetCurrent%20Rotation%20Speed)) (Math|Float|Power (Math|Float|Absolute(Float) (Variables|Default|GetCurrent%20Rotation%20Speed)) (Variables|Speed|GetSpeedShip))))
      (Development|PrintString (Utilities|String|ToString(Float) (Variables|Speed|GetSpeedShip))))))

(event EventCameraLook
  (params (LookDirection :type Vector%202D%20Structure))
  (bind _current_rotation_speed (Variables|Default|GetCurrent%20Rotation%20Speed))
  ;[0.4203 0.3757 1] Set Rotation
  (Variables|Default|SetIs%20Rotate true)
  (Transformation|AddActorLocalRotation (Math|Rotator|MakeRotator 0.0 (* (.y LookDirection) _current_rotation_speed) (* (.x LookDirection) _current_rotation_speed)) false false))

(event EventMoveBack
  (params (Value :type Float%20%28double-precision%29))
  ;[0.9969 1 0.5568] Move Forward
  (Variables|Default|SetBack%20Movement true)
  (Variables|Default|SetForward%20Movement false)
  (Variables|Speed|SetSpeedShip (Math|Interpolation|FInterpTo (Variables|Speed|GetSpeedShip) (* Value (Variables|Speed|GetspeedMax_Back)) (Utilities|Time|GetWorldDeltaSeconds) 1.0)))

(event EventMoveForward
  (params (Value :type Float%20%28double-precision%29))
  ;[0.9969 1 0.5568] Move Forward
  (Variables|Default|SetForward%20Movement true)
  (Variables|Default|SetBack%20Movement false)
  (Variables|Speed|SetSpeedShip (Math|Interpolation|FInterpTo (Variables|Speed|GetSpeedShip) (* Value (Variables|Speed|GetspeedMax_Forward)) (Utilities|Time|GetWorldDeltaSeconds) 0.5)))

(fn ConstructionScript)

(fn RollShip
  (params (DeltaTime :type Float%20%28single-precision%29) (Right%20Float :type Float%20%28double-precision%29) (Up%20Float :type Float%20%28double-precision%29))
  (if (!= Right%20Float 0.0)
    (if (> (Variables|Speed|GetShipStop) 0.01)
      (if (> (Variables|Speed|GetSpeedShip) 0.0)
        (|PositiveRoll DeltaTime Right%20Float Up%20Float)
        (return)
        (else
          (|NegativeRoll Right%20Float DeltaTime Up%20Float)
          (return)))
      (else
        (|ResetRotationto0 (Variables|Default|GetSPA_Ship) DeltaTime)
        (return)))
    (else
      (|ResetRoll (Variables|Default|GetSPA_Ship) DeltaTime)
      (return))))

(fn MoveShipbySpeed
  (bind _pointreferencemesh (Variables|Default|GetPointReferenceMesh))
  (bind _returnvalue (Physics|GetPhysicsLinearVelocity _pointreferencemesh "None"))
  (Physics|SetPhysicsLinearVelocity _pointreferencemesh (Math|Vector|Lerp(Vector) _returnvalue (* (Transformation|GetActorForwardVector) (* (* (Variables|Speed|GetSpeedShip) (.speedmax (Variables|Speed|GetSpeedParameters))) (Variables|Speed|GetShipStop))) 0.01) false "None"))

(fn Brake
  (CallFunction|DecreaseValueinTime (Variables|Speed|GetSpeedShip) 0.0 0.0 1.0 0.0 0.0 false)
  (CallFunction|DecreaseValueExp 0.0 1.0 1.0 1.1 0.0))