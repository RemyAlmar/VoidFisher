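; BP_PC_Flight is the player controller for ship flight, translating Enhanced Input actions into commands for the player pawn.
; On BeginPlay it adds the Ship_Controller mapping context, then forwards acceleration, deceleration, vertical movement, roll, camera look and rotation-mode switching as message calls to player pawn 0.
; Roll, camera look and rotation-mode inputs forward on both Triggered and Completed, so the pawn also receives the release value.
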(event Input|EnhancedActionEvents|EnhancedInputActionIA_CameraLook
  (params (ActionValue :type Vector%202D%20Structure) (ElapsedSeconds :type Float%20%28double-precision%29) (TriggeredSeconds :type Float%20%28double-precision%29) (InputAction :type Input%20Action%20Object%20Reference :default "/Game/Blueprints/Player/Controllers/InputsActions/IA_CameraLook.IA_CameraLook"))
  (:Triggered
    (Class|BPIMoveable|CameraLook(Message) (Game|Player|GetPlayerPawn 0) ActionValue :!label _label))
  (:Completed
    (goto _label)))

(event Input|EnhancedActionEvents|EnhancedInputActionIA_Accelerate
  (params (ActionValue :type Float%20%28double-precision%29) (ElapsedSeconds :type Float%20%28double-precision%29) (TriggeredSeconds :type Float%20%28double-precision%29) (InputAction :type Input%20Action%20Object%20Reference :default "/Game/Blueprints/Player/Controllers/InputsActions/IA_Accelerate.IA_Accelerate"))
  (Class|BPIMoveable|MoveForward(Message) (Game|Player|GetPlayerPawn 0) ActionValue))

(event Input|EnhancedActionEvents|EnhancedInputActionIA_Decelerate
  (params (ActionValue :type Float%20%28double-precision%29) (ElapsedSeconds :type Float%20%28double-precision%29) (TriggeredSeconds :type Float%20%28double-precision%29) (InputAction :type Input%20Action%20Object%20Reference :default "/Game/Blueprints/Player/Controllers/InputsActions/IA_Decelerate.IA_Decelerate"))
  (Class|BPIMoveable|MoveBack(Message) (Game|Player|GetPlayerPawn 0) ActionValue))

(event Input|EnhancedActionEvents|EnhancedInputActionIA_SwitchRotationMode
  (params (ActionValue :type Boolean) (ElapsedSeconds :type Float%20%28double-precision%29) (TriggeredSeconds :type Float%20%28double-precision%29) (InputAction :type Input%20Action%20Object%20Reference :default "/Game/Blueprints/Player/Controllers/InputsActions/IA_SwitchRotationMode.IA_SwitchRotationMode"))
  (:Triggered
    (Class|BPIMoveable|SwitchRotationMode(Message) (Game|Player|GetPlayerPawn 0) ActionValue :!label _label))
  (:Completed
    (goto _label)))

(event Input|EnhancedActionEvents|EnhancedInputActionIA_HorizontalRoll
  (params (ActionValue :type Float%20%28double-precision%29) (ElapsedSeconds :type Float%20%28double-precision%29) (TriggeredSeconds :type Float%20%28double-precision%29) (InputAction :type Input%20Action%20Object%20Reference :default "/Game/Blueprints/Player/Controllers/InputsActions/IA_HorizontalRoll.IA_HorizontalRoll"))
  (:Triggered
    (Class|BPIMoveable|HorizontalRoll(Message) (Game|Player|GetPlayerPawn 0) ActionValue :!label _label))
  (:Completed
    (goto _label)))

(event Input|EnhancedActionEvents|EnhancedInputActionIA_VertialMovement
  (params (ActionValue :type Float%20%28double-precision%29) (ElapsedSeconds :type Float%20%28double-precision%29) (TriggeredSeconds :type Float%20%28double-precision%29) (InputAction :type Input%20Action%20Object%20Reference :default "/Game/Blueprints/Player/Controllers/InputsActions/IA_VertialMovement.IA_VertialMovement"))
  (Class|BPIMoveable|VerticalMovement(Message) (Game|Player|GetPlayerPawn 0) ActionValue))

(event EventBeginPlay
  (bind _self self)
  (bind _returnvalue (PlayerController|LocalPlayerSubsystems|GetEnhancedInputLocalPlayerSubsystem _self))
  (Utilities|IsValid _returnvalue
    (:Is%20Valid
      (Input|AddMappingContext _returnvalue "/Game/Blueprints/Player/Controllers/InputsActions/Ship_Controller.Ship_Controller" 0 "(bIgnoreAllPressedKeysUntilRelease=True,bForceImmediately=False,bNotifyUserSettings=False)"))))

(fn ConstructionScript)