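; Test player pawn for a physics-driven ship that steers by torque, with a toggle between roll and yaw.
; Forward and back inputs switch a BP_StateCommander state machine, reverting after a short retriggerable delay, while interface events ramp throttle, brake and speed.
; Tick updates the commander, damps spin with counter-torque and blends velocity toward the ship's forward vector.
; Camera look slows near clamp limits around its starting rotation and eases back when input stops.
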(event Custom|NoAcceleration
  (bind _basevehicleoptions (Variables|StructureVehiculeOptions|GetBaseVehicleOptions))
  ;[0 1 0.05186] Vehicle Neutral State
  (CallFunction|DecreaseValueinTime (Variables|VehicleParametres|GetCurrentThrottle) (Variables|VehicleParametres|GetCurrentThrottleTime) 0.0 3.0 (.throttletimemax _basevehicleoptions) (.throttlemax _basevehicleoptions) false))

(event Custom|NoBrake
  (bind _basevehicleoptions (Variables|StructureVehiculeOptions|GetBaseVehicleOptions))
  ;[0 1 0.05186] Vehicle Neutral State
  (CallFunction|DecreaseValueinTime (Variables|VehicleParametres|GetCurrentBrake) (Variables|VehicleParametres|GetCurrentBrakeTime) 0.0 3.0 (.throttletimemax _basevehicleoptions) (.brakepowermax _basevehicleoptions) false))

(event EventBeginPlay
  (AddComponent|AddChildActorComponent false) ; set HUD
  (bind _returnvalue (Game|ConstructObjectfromClass "/Game/Blueprints/Commander/BP_StateCommander.BP_StateCommander_C"))
  (Variables|VehicleStates|SetVehicleStateCommand _returnvalue)
  (bind _statelist (CallFunction|ConstructState (Variables|VehicleStates|GetVehicleStatesListClass)))
  (Default|InititalizeCommander (Variables|VehicleStates|GetVehicleStateCommand) self _statelist (Utilities|Enum|LiteralenumE_VehicleState "NewEnumerator2"))
  (Variables|Camera|SetCameraTransform (Transformation|GetRelativeTransform (Variables|Default|GetSpringArm)))
  (Variables|Camera|SetLagSpeedBase (Variables|/Script/Engine.SpringArmComponent|GetCameraLagSpeed (Variables|Default|GetSpringArm)))
  (Variables|Camera|SetblsCamWasReset true)
  (Variables|Camera|SetrttCamRotationRT (Variables|/Script/Engine.SceneComponent|GetRelativeRotation (Variables|Default|GetCamera)))
  (|SetMaxClampVariables))

(event EventIRegresseable
  (bind _basevehicleoptions (Variables|StructureVehiculeOptions|GetBaseVehicleOptions))
  ;[0 1 0.05186] Recule
  (bind _currentvaluetoincrease (CallFunction|IncreaseValueinTime (Variables|VehicleParametres|GetCurrentBrake) (Variables|VehicleParametres|GetCurrentBrakeTime) (stale EventMoveBack Value) (.brakepowermax _basevehicleoptions) (.braketimemax _basevehicleoptions) false))
  (CallFunction|NoAcceleration)
  (CallFunction|DecreaseValueExp (Variables|VehicleParametres|GetCurrentSpeed) (stale EventMoveBack Value) _currentvaluetoincrease 1.05 (.speedmax (Variables|StructureVehiculeOptions|GetBaseVehicleOptions))))

(event EventSwitchRotationMode
  (params (boolvalue :type Boolean))
  ;[0 1 0.3717] Movement
  (Variables|RollsFlight|SetIsRollingMode boolvalue))

(event EventIThrottle
  (bind _basevehicleoptions (Variables|StructureVehiculeOptions|GetBaseVehicleOptions))
  ;[0 1 0.05186] Accelerate
  (bind _currentvaluetoincrease (CallFunction|IncreaseValueinTime (Variables|VehicleParametres|GetCurrentThrottle) (Variables|VehicleParametres|GetCurrentThrottleTime) (stale EventMoveForward Value) (.throttlemax _basevehicleoptions) (.throttletimemax _basevehicleoptions) false))
  (CallFunction|NoBrake)
  (CallFunction|IncreaseValueExp (Variables|VehicleParametres|GetCurrentSpeed) (stale EventMoveForward Value) _currentvaluetoincrease 1.1 (.speedmax (Variables|StructureVehiculeOptions|GetBaseVehicleOptions))))

(event EventMoveForward
  (params (Value :type Float%20%28double-precision%29))
  ;[0 1 0.05186] Accelerate
  (Default|ChangeState (Variables|VehicleStates|GetVehicleStateCommand) (Utilities|Enum|LiteralenumE_VehicleState "NewEnumerator0"))
  (Utilities|FlowControl|RetriggerableDelay 0.2)
  (Default|ChangeState (Variables|VehicleStates|GetVehicleStateCommand) (Utilities|Enum|LiteralenumE_VehicleState "NewEnumerator2")))

(event EventMoveBack
  (params (Value :type Float%20%28double-precision%29))
  ;[0 1 0.05186] Recule
  (Default|ChangeState (Variables|VehicleStates|GetVehicleStateCommand) (Utilities|Enum|LiteralenumE_VehicleState "NewEnumerator1"))
  (Utilities|FlowControl|RetriggerableDelay 0.1)
  (Default|ChangeState (Variables|VehicleStates|GetVehicleStateCommand) (Utilities|Enum|LiteralenumE_VehicleState "NewEnumerator2")))

(event EventVerticalMovement
  (params (AxisValue :type Float%20%28double-precision%29))
  ;[0 1 0.3717] Movement
  (CallFunction|TorqueMotion AxisValue (.maniability (Variables|StructureVehiculeOptions|GetBaseVehicleOptions)) (Math|Vector|GetRightVector (Variables|Default|GetShip_Temp))))

(event EventCameraLook
  (params (LookDirection :type Vector%202D%20Structure))
  (bind _camera (Variables|Default|GetCamera))
  (bind _relativerotation (Variables|/Script/Engine.SceneComponent|GetRelativeRotation _camera))
  (bind _result____ (CallFunction|SmoothClamp (.pitch _relativerotation) (Variables|Default|GetMin%20Pitch) (Variables|Default|GetMaxPitch))) ; Pitch
  (bind _result_____2 (CallFunction|SmoothClamp (.yaw _relativerotation) (Variables|Default|GetMax%20Yaw) (Variables|Default|GetMin%20Yaw))) ; Yaw
  (Variables|Camera|SetblsCamWasReset false)
  (Transformation|AddRelativeRotation (Variables|Default|GetCamera) (Math|Rotator|MakeRotator 0.0 (* (* (.y LookDirection) _result____) -1.0) (* (.x LookDirection) _result_____2)) false false) ; Simple Rotation
  (Transformation|SetRelativeRotation (Variables|Default|GetCamera) (Math|Rotator|MakeRotator 0.0 (Math|Float|Clamp(Float) (.pitch _relativerotation) (Variables|Default|GetMin%20Pitch) (Variables|Default|GetMaxPitch)) (Math|Float|Clamp(Float) (.yaw _relativerotation) (Variables|Default|GetMin%20Yaw) (Variables|Default|GetMax%20Yaw))) false false) ; Clamp Rotation
  (Utilities|FlowControl|RetriggerableDelay 0.1)
  (Variables|Camera|SetblsCamWasReset true))

(event EventHorizontalMovement
  (params (AxisValue :type Float%20%28double-precision%29))
  ;[0 1 0.3717] Movement
  (CallFunction|TorqueMotion (CallFunction|InverseInput (Variables|RollsFlight|GetIsRollingMode) AxisValue) (.maniability (Variables|StructureVehiculeOptions|GetBaseVehicleOptions)) (CallFunction|GetRollsVector)))

(event EventTick
  (params (DeltaSeconds :type Float%20%28single-precision%29))
  (bind _camera (Variables|Default|GetCamera))
  (Default|Update (Variables|VehicleStates|GetVehicleStateCommand))
  (Class|PrimitiveComponent|AddTorqueinDegrees (Variables|Default|GetShip_Temp) (/ (Math|Vector|NegateVector (Physics|GetPhysicsAngularVelocityinDegrees (Variables|Default|GetShip_Temp) "None")) 0.2) "None" true)
  (CallFunction|CalculateSpeed)
  (Pawn|SetControlRotation (Game|GetPlayerController 0) (Pawn|GetControlRotation :!class /Script/Engine.Pawn))
  (if (Variables|Camera|GetblsCamWasReset)
    (Transformation|SetRelativeRotation _camera (Math|Interpolation|RInterpTo (Variables|/Script/Engine.SceneComponent|GetRelativeRotation _camera) (Variables|Camera|GetrttCamRotationRT) DeltaSeconds 2.0) false false)))

(event EventIDeceleration
  ;[0 1 0.05186] Vehicle Neutral State
  (CallFunction|NoAcceleration)
  (CallFunction|NoBrake))

(fn ConstructionScript)

(fn ThrottleForward
  (params (Value :type Float%20%28double-precision%29))
  (return (* Value (Transformation|GetActorForwardVector))))

(fn ConstructState
  (params (E_Type :type Map%20of%20Bytes%20to%20Classs))
  (bind _keys (Utilities|Map|Keys E_Type))
  (for _array_element _keys
    (bind _returnvalue (Game|ConstructObjectfromClass (.Value (Utilities|Map|Find E_Type _array_element))))
    (Utilities|Map|Add (LocalVariables|GetStatesList) _array_element _returnvalue))
  (return (LocalVariables|GetStatesList)))

(fn TorqueMotion
  (params (InputValue :type Float%20%28double-precision%29) (MultiplierSpeed :type Float%20%28double-precision%29) (VectorDirection :type Vector))
  (Class|PrimitiveComponent|AddTorqueinDegrees (Variables|Default|GetShip_Temp) (Math|Vector|Lerp(Vector) "0, 0, 0" (* VectorDirection (* InputValue MultiplierSpeed)) 0.1) "None" true))

(fn GetRollsVector
  (if (Variables|RollsFlight|GetIsRollingMode)
    (LocalVariables|SetRollsVector (Math|Vector|GetForwardVector (Variables|Default|GetShip_Temp)))
    (else
      (LocalVariables|SetRollsVector (Math|Vector|GetUpVector (Variables|Default|GetShip_Temp)))))
  (return (LocalVariables|GetRollsVector)))

(fn CalculateSpeed
  (bind _returnvalue (Physics|GetPhysicsLinearVelocity (Variables|Default|GetShip_Temp) "None"))
  (Physics|SetPhysicsLinearVelocity (Variables|Default|GetShip_Temp) (Math|Vector|Lerp(Vector) _returnvalue (* (Math|Vector|GetForwardVector (Variables|Default|GetShip_Temp)) (Variables|VehicleParametres|GetCurrentSpeed)) 0.01) false "None"))

(fn InverseInput
  (params (Bool :type Boolean) (Input :type Float%20%28double-precision%29%20%28by%20ref%29))
  (if Bool
    _
    (else
      (Math|Float|NegateFloat Input
        (:%20%20
          _))))
  (return Input))

(fn ControlCamera
  (params (CameraRotation :type Vector%202D%20Structure))
  (Pawn|Input|AddControllerYawInput (* (Variables|Camera|GetSpeedMultiplierRotation) (.x CameraRotation)))
  (Pawn|Input|AddControllerPitchInput (* (Variables|Camera|GetSpeedMultiplierRotation) (.y CameraRotation)))
  (Variables|/Script/Engine.SpringArmComponent|SetCameraLagSpeed (Variables|Default|GetSpringArm) 0.0))

(fn ControlFreeCamera
  (params (InputValue :type Vector%202D%20Structure))
  (bind _springarm (Variables|Default|GetSpringArm))
  (bind _springarm_2 (Variables|Default|GetSpringArm))
  (bind _relativerotation (Variables|/Script/Engine.SceneComponent|GetRelativeRotation _springarm_2))
  (Variables|/Script/Engine.SpringArmComponent|SetbInheritYaw _springarm false)
  (Variables|/Script/Engine.SpringArmComponent|SetbInheritPitch _springarm false)
  (Variables|/Script/Engine.SpringArmComponent|SetbInheritRoll _springarm false)
  (if (Variables|Camera|GetblsCamWasReset)
    ;[0 0 0] Set la position initiale par rapport au vaisseau
    (Variables|Camera|SetblsCamWasReset false)
    (bind _output_get (Variables|Camera|SetRollRotator (Math|Rotator|Delta(Rotator) (Transformation|GetWorldRotation (Variables|Default|GetSpringArm)) (Math|Rotator|FindLookatRotation (Transformation|GetWorldLocation (Variables|Default|GetSpringArm)) (Transformation|GetWorldLocation (Variables|Default|GetShip_Temp))))))
    (bind _output_get_2 (Variables|Camera|SetrttCamRotationRT _output_get))
    (Transformation|AddRelativeRotation (Variables|Default|GetSpringArm) (Math|Rotator|MakeRotator (.roll _output_get_2) (.pitch _output_get_2) (.yaw _output_get_2)) false false)
    (Variables|Camera|SetblsFreeCamActive true))
  (Transformation|AddRelativeRotation _springarm_2 (Math|Rotator|MakeRotator 0.0 (.y InputValue) (.x InputValue)) false false)
  (Transformation|SetRelativeRotation _springarm_2 (Math|Rotator|MakeRotator (.roll _relativerotation) (Math|Float|Clamp(Float) (.pitch _relativerotation) -7e+01 7e+01) (.yaw _relativerotation)) true false)
  (Development|PrintString (Utilities|String|ToString(Rotator) (Variables|/Script/Engine.SceneComponent|GetRelativeRotation _springarm_2))))

(fn ResetCameraPosition)

(fn SmoothClamp
  (params (Relative%20Rotation :type Float%20%28double-precision%29) (Max%20Clamp :type Float%20%28double-precision%29) (Min%20Clap :type Float%20%28double-precision%29))
  (return (/ (Math|Float|Min(Float) (- Max%20Clamp Relative%20Rotation) (- Relative%20Rotation Min%20Clap)) (- Max%20Clamp Min%20Clap))))