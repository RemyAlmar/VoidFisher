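; BP_ToolLauncher is a player tool that spawns and launches a configurable projectile.
; Use spawns it at SpawnTransform with random power and scale multipliers, then launches it forward, passing the owner's velocity.
; Secondary use activates the last spawned projectile.
; UpdateStat multiplies a selected stat: that projectile's radius or power, or the tool's launch power.
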(event EventUse
  (bind _returnvalue (Math|Random|RandomFloatinRange 2.0 1e+01))
  (bind _spawntransform (Variables|Default|GetSpawnTransform))
  (bind _returnvalue_2 (Game|SpawnActorfromClass (Variables|ObjectToSpawn|GetObjectToSpawn) (Transformation|GetWorldTransform _spawntransform) "Undefined" "MultiplyWithRoot" 0 0))
  (bind _output_get (Variables|ObjecttoSpawn|SetObject _returnvalue_2))
  (Default|Initialize _output_get _returnvalue _returnvalue)
  (CallFunction|LaunchActor _output_get (Math|Vector|GetForwardVector _spawntransform) (Variables|Statistiques|GetLauncherPower) (Transformation|GetVelocity (Components|GetOwner))))

(event EventInitialize
  (|CallParentFunction))

(event EventActive
  (|CallParentFunction))

(event EventDeactive
  (|CallParentFunction))

(event EventUseSecondary
  (Default|ActivationProjectile (Variables|ObjecttoSpawn|GetObject)))

(fn UpdateStat
  (params (Selection :type E_StatUpgrade%20Enum :default "NewEnumerator0") (Multiplier :type Float%20%28double-precision%29))
  (bind _object (Variables|ObjecttoSpawn|GetObject))
  (bind _launcherpower (Variables|Statistiques|GetLauncherPower))
  (switch Utilities|FlowControl|Switch|SwitchonE_StatUpgrade Selection
    (:NewEnumerator0
      (Default|ChangeScale (Variables|ObjecttoSpawn|GetObject) Multiplier))
    (:NewEnumerator1
      (Default|ChangeFloatStat _object (Variables|/Game/Blueprints/Spawnables/BP_Projectile.BP_Projectile_C|GetPower _object) Multiplier) ; Faire un node generique de ca
    )
    (:NewEnumerator2
      (|SetBy-RefVar _launcherpower (* _launcherpower Multiplier)))))