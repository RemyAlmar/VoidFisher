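; Player net tool Blueprint that detects catchable actors through a box collider.
; Activation shows the collider and enables overlap events, deactivation reverses both, and each calls its parent.
; While the tool is in use, overlaps with Catcheable actors only print the name and weight from their data message.
; UpdateStat's Radius case scales the box's Y and Z extents, leaving X unchanged.
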(event Custom|Overlap
  (params (OverlappedComponent :type Primitive%20Component%20Object%20Reference) (OtherActor :type Actor%20Object%20Reference) (OtherComp :type Primitive%20Component%20Object%20Reference) (OtherBodyIndex :type Integer) (bFromSweep :type Boolean) (SweepResult :type Hit%20Result%20Structure%20%28by%20ref%29))
  (if (Variables|Default|GetIsUsed)
    (Development|PrintText "ActorOverlap" true true "(R=0.000000,G=0.660000,B=1.000000,A=1.000000)" 5.0)
    (if (Utilities|DoesObjectImplementInterface OtherActor "/Script/VoidFisher.Catcheable")
      (bind _returnvalue (Class|Catcheable|GetData(Message) OtherActor))
      (Development|PrintText (Utilities|Text|FormatText "{name} Added  
It weighs {weight} Kg;" (.name _returnvalue) (.size _returnvalue))))
    (else
      (Development|PrintText "NotUsed" true true "(R=0.000000,G=0.660000,B=1.000000,A=1.000000)" 5.0))))

(event EventActive
  (Development|SetHiddeninGame (Variables|Default|GetNetCollider) false false)
  (Variables|/Script/Engine.PrimitiveComponent|SetbGenerateOverlapEvents (Variables|Default|GetNetCollider) true)
  (|CallParentFunction))

(event EventDeactive
  (Development|SetHiddeninGame (Variables|Default|GetNetCollider) true true)
  (Variables|/Script/Engine.PrimitiveComponent|SetbGenerateOverlapEvents (Variables|Default|GetNetCollider) false)
  (|CallParentFunction))

(event EventUse
  (|CallParentFunction))

(event EventInitialize
  (Collision|BindEventtoOnComponentBeginOverlap (Variables|Default|GetNetCollider) (EventDispatchers|CreateEvent :!event Custom|Overlap))
  (|CallParentFunction))

(fn UpdateStat
  (params (Selection :type E_StatUpgrade%20Enum :default "NewEnumerator0") (Multiplier :type Float%20%28double-precision%29))
  (bind _netcollider (Variables|Default|GetNetCollider))
  (bind _boxextent (Variables|/Script/Engine.BoxComponent|GetBoxExtent _netcollider))
  (bind _returnvalue (* Multiplier _boxextent))
  (switch Utilities|FlowControl|Switch|SwitchonE_StatUpgrade Selection
    (:NewEnumerator0
      (Components|Box|SetBoxExtent _netcollider (Math|Vector|MakeVector (/ (.x _returnvalue) Multiplier) (.y _returnvalue) (.z _returnvalue)) true))))