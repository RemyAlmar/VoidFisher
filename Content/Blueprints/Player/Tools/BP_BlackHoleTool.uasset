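; Player tool that launches a black hole object and triggers it on secondary use, extending a parent tool class.
; Use spawns the object with random radius and gravity, then launches it forward, passing the owner's velocity.
; Only the latest spawn is stored, so activation and radius or gravity stat changes target that object.
; UpdateStat can also scale the tool's launch power.
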(event EventUse
  (bind _returnvalue (Math|Random|RandomFloatinRange 2.0 1e+01))
  (bind _spawntransform (Variables|Default|GetSpawnTransform))
  (bind _returnvalue_2 (Game|SpawnActorfromClass (Variables|Default|GetTestObject) (Transformation|GetWorldTransform _spawntransform) "Undefined" "MultiplyWithRoot" 0 0))
  (bind _output_get (Variables|Default|SetBlackHoleObject _returnvalue_2))
  (Default|Initialize _output_get _returnvalue (* _returnvalue 1e+02))
  (CallFunction|LaunchActor _output_get (Math|Vector|GetForwardVector _spawntransform) (Variables|Statistiques|GetLauncherPower) (Transformation|GetVelocity (Components|GetOwner))))

(event EventInitialize
  (|CallParentFunction))

(event EventActive
  (|CallParentFunction))

(event EventDeactive
  (|CallParentFunction))

(event EventUseSecondary
  (Default|ActivateBlackHole (Variables|Default|GetBlackHoleObject)))

(fn UpdateStat
  (params (Selection :type E_StatUpgrade%20Enum :default "NewEnumerator0") (Multiplier :type Float%20%28double-precision%29))
  (bind _blackholeobject (Variables|Default|GetBlackHoleObject))
  (bind _launcherpower (Variables|Statistiques|GetLauncherPower))
  (switch Utilities|FlowControl|Switch|SwitchonE_StatUpgrade Selection
    (:NewEnumerator0
      (Default|ChangeGlobalRadius (Variables|Default|GetBlackHoleObject) Multiplier))
    (:NewEnumerator1
      (Default|ChangeGravityPower _blackholeobject (* (Default|GetCurrentGravityPower _blackholeobject) Multiplier)))
    (:NewEnumerator2
      (|SetBy-RefVar _launcherpower (* Multiplier _launcherpower)))))