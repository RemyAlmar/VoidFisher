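; BP_SuckerTool is a player tool that spawns and launches a sucker object when used.
; Use spawns a TestObject at the spawn transform, initializes it with a random float, and launches it forward using LauncherPower and the owner's velocity.
; UpdateStat scales LauncherPower by a multiplier, compounding on each call.
; Initialize, Active and Deactive only call their parent versions, and secondary use is empty.
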(event EventUse
  (bind _spawntransform (Variables|Default|GetSpawnTransform))
  (bind _returnvalue (Game|SpawnActorfromClass (Variables|Default|GetTestObject) (Transformation|GetWorldTransform _spawntransform) "Undefined" "MultiplyWithRoot" 0 0))
  (bind _output_get (Variables|Default|SetSuckerObject _returnvalue))
  (Default|Initialize _output_get (Math|Random|RandomFloatinRange 2.0 1e+01))
  (CallFunction|LaunchActor _output_get (Math|Vector|GetForwardVector _spawntransform) (Variables|Statistiques|GetLauncherPower) (Transformation|GetVelocity (Components|GetOwner))))

(event EventInitialize
  (|CallParentFunction))

(event EventActive
  (|CallParentFunction))

(event EventDeactive
  (|CallParentFunction))

(event EventUseSecondary)

(fn UpdateStat
  (params (Selection :type E_StatUpgrade%20Enum :default "NewEnumerator0") (Multiplier :type Float%20%28double-precision%29))
  (bind _launcherpower (Variables|Statistiques|GetLauncherPower))
  (switch Utilities|FlowControl|Switch|SwitchonE_StatUpgrade Selection
    (:NewEnumerator2
      (|SetBy-RefVar _launcherpower (* Multiplier _launcherpower)))))