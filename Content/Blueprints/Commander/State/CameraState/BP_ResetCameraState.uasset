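; BP_ResetCameraState is a Commander camera state, named for resetting the camera.
; On every Update it sends the IRegresseable interface message to its Target, then runs the parent logic.
; Start, Quit and ChangeState defer to the parent state.
; Start, Update and Quit also print debug strings that are labeled "Brake" rather than reset.
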(event EventStart
  (Development|PrintString 0 "StartBrake" true true "(R=0.000000,G=0.149016,B=1.000000,A=1.000000)")
  (|CallParentFunction))

(event EventUpdate
  (Development|PrintString 0 "UpdateBrake" true true "(R=0.000000,G=1.000000,B=0.000306,A=1.000000)" 0.0)
  (Class|BPIVehicleHandleable|IRegresseable(Message) (Variables|Default|GetTarget))
  (|CallParentFunction))

(event EventQuit
  (Development|PrintString 0 "QuitBrake" true true "(R=1.000000,G=0.036022,B=0.135688,A=1.000000)")
  (|CallParentFunction))

(event EventChangeState
  (params (TargetState :type Byte :default 0))
  (|CallParentFunction TargetState))