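; BP_State is a state for the Commander's state machine, apparently meant as a base for concrete states.
; It holds a target, a name and its Commander, all assigned through InitState.
; OnProcess switches on a Start/Update/Quit phase to call the matching event; Start advances to Update, while Update and Quit are empty.
; ChangeState forwards transition requests to the Commander, and SetState sets the phase directly.
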(event EventStart
  (Variables|Default|SetStateOfState "NewEnumerator1"))

(event EventUpdate)

(event EventQuit)

(event EventChangeState
  (params (TargetState :type Byte :default 0))
  (Default|ChangeState (Variables|Default|GetCommander) TargetState))

(event EventOnProcess
  (switch Utilities|FlowControl|Switch|SwitchonE_StateMachine (Variables|Default|GetStateOfState)
    (:NewEnumerator0
      (CallFunction|Start))
    (:NewEnumerator1
      (CallFunction|Update))
    (:NewEnumerator2
      (CallFunction|Quit))))

(fn InitState
  (params (Target :type Actor%20Object%20Reference) (StateName :type Byte) (Commander :type BP%20State%20Commander%20Object%20Reference))
  (Variables|Default|SetTarget Target)
  (Variables|Default|SetStateName StateName)
  (Variables|Default|SetCommander Commander))

(fn SetState
  (params (StateOfState :type E_StateMachine%20Enum :default "NewEnumerator0"))
  (Variables|Default|SetStateOfState StateOfState))