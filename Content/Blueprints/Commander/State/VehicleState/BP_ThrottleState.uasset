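; BP_ThrottleState is a vehicle state in the commander's state system that handles throttling.
; Each update it sends the IThrottle interface message to its Target, then runs the parent update.
; Start, Quit and ChangeState defer to the parent class, with debug prints marking start, update and quit.
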(event EventStart
  (Development|PrintString 0 "StartThrottle" true true "(R=0.000000,G=0.073006,B=1.000000,A=1.000000)")
  (|CallParentFunction))

(event EventUpdate
  (Development|PrintString 0 "UpdateThrottle" true true "(R=0.099820,G=1.000000,B=0.000000,A=1.000000)" 0.0)
  (Class|BPIVehicleHandleable|IThrottle(Message) (Variables|Default|GetTarget))
  (|CallParentFunction))

(event EventQuit
  (Development|PrintString 0 "QuitThrottle" true true "(R=1.000000,G=0.156285,B=0.000000,A=1.000000)" 1.0)
  (|CallParentFunction))

(event EventChangeState
  (params (TargetState :type Byte :default 0))
  (|CallParentFunction TargetState))