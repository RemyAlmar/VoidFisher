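; BP_NeutralState is the neutral state in the Commander's vehicle state set.
; Start, Update, Quit and ChangeState all pass through to the parent state implementation, with debug prints on the first three.
; Its only behavior of its own is in Update, which sends IDecelerationMessage to the Target so it decelerates while in neutral.
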(event EventStart
  (Development|PrintString 0 "StartNeutral" true true "(R=0.000000,G=0.121732,B=1.000000,A=1.000000)")
  (|CallParentFunction))

(event EventUpdate
  (Development|PrintString 0 "UpdateNeutral" true true "(R=0.105208,G=1.000000,B=0.000000,A=1.000000)" 0.0)
  (Class|BPIVehicleHandleable|IDeceleration(Message) (Variables|Default|GetTarget))
  (|CallParentFunction))

(event EventQuit
  (Development|PrintString 0 "QuitNeutral" true true "(R=1.000000,G=0.000000,B=0.129005,A=1.000000)")
  (|CallParentFunction))

(event EventChangeState
  (params (TargetState :type Byte :default 0))
  (|CallParentFunction TargetState))