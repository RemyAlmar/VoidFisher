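; BP_StateCommander is a finite state machine that manages a map of enum-keyed state objects for a given target.
; InititalizeCommander stores the map, gives each state the target, its name and a commander back-reference, then picks the start state without calling SetState.
; Update forwards processing to the current state.
; ChangeState ignores the active state, otherwise calling SetState on outgoing and incoming states around the swap.
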(event EventUpdate
  (Default|OnProcess (Variables|State|GetCurrentState)))

(event EventChangeState
  (params (TargetState :type Byte :default 0))
  (if (not (CallFunction|AlreadyinState TargetState))
    (Default|SetState (Variables|State|GetCurrentState) "NewEnumerator2")
    (bind _output_get (Variables|State|SetCurrentState (.Value (Utilities|Map|Find (Variables|State|GetListStates) TargetState))))
    (Default|SetState _output_get "NewEnumerator0")))

(fn InitStates
  (bind _keys (Utilities|Map|Keys (Variables|State|GetListStates)))
  (for _array_element _keys
    (Default|InitState (.Value (Utilities|Map|Find (Variables|State|GetListStates) _array_element)) (Variables|Target|GetTarget) _array_element self))
  (return))

(fn AddState
  (params (E_State :type Byte%20%28by%20ref%29) (State :type BP%20State%20Object%20Reference%20%28by%20ref%29))
  (Utilities|Map|Add (Variables|State|GetListStates) E_State State))

(fn InititalizeCommander
  (params (Target :type Actor%20Object%20Reference) (ListStates :type Map%20of%20Bytes%20to%20Objects) (StartState :type Byte%20%28by%20ref%29))
  (Variables|Target|SetTarget Target)
  (Variables|State|SetListStates ListStates)
  (CallFunction|InitStates)
  (Variables|State|SetCurrentState (.Value (Utilities|Map|Find (Variables|State|GetListStates) StartState))))

(fn GetCurrentState
  (return (.Value (Utilities|Map|Find (Variables|State|GetListStates) (Variables|/Game/Blueprints/Commander/State/BP_State.BP_State_C|GetStateName (Variables|State|GetCurrentState))))))

(fn GetAnyState
  (params (State :type Byte))
  (return (.Value (Utilities|Map|Find (Variables|State|GetListStates) State))))

(fn DisplayStates
  (bind _keys (Utilities|Map|Keys (Variables|State|GetListStates)))
  (for _array_element _keys
    (if (.ReturnValue (Utilities|Map|Find (Variables|State|GetListStates) _array_element))
      (Development|PrintText 0 (Utilities|Text|FormatText "{StateName} = {StateObject}" _array_element (Utilities|GetDisplayName (.Value (Utilities|Map|Find (Variables|State|GetListStates) _array_element)))))
      (else
        (Development|PrintString 0 "Dont FOund"))))
  (return))

(fn AlreadyinState
  (params (State :type Byte))
  (return (== (.Value (Utilities|Map|Find (Variables|State|GetListStates) State)) (Variables|State|GetCurrentState))))