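; BP_Sucker is a spawnable black hole actor that arms itself after a delay and destroys itself when its lifetime runs out.
; Tick runs two TimerPos timers: one triggers activation once through a DoOnce, the other destroys the actor.
; Initialize sets a uniform scale from a multiplier.
; The ActiveSucker function called on BeginPlay and activation is empty, so activation only sets a flag and prints debug text.
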(event Custom|ActivateSucker
  (if (not (Variables|Default|GetbActiveSucker))
    (bind _output_get (Variables|Default|SetbActiveSucker true))
    (CallFunction|ActiveSucker _output_get)
    (Development|PrintString "ActivationBlackHoleSelf" true true "(R=0.044169,G=1.000000,B=0.000000,A=1.000000)" 5.0)))

(event EventBeginPlay
  (CallFunction|ActiveSucker (Variables|Default|GetbActiveSucker))
  (Development|PrintString "Apparition Trou Noir"))

(event EventTick
  (params (DeltaSeconds :type Float%20%28single-precision%29))
  (Utilities|FlowControl|Sequence
    (:then_0
      (if (not (Variables|Default|GetbActiveSucker))
        (if (CallFunction|TimerPos (Variables|Default|GetTriggerTimeCurrent) (Variables|Default|GetTriggerTimeMax) 1.0 false)
          (Utilities|FlowControl|DoOnce false
            (:Completed
              (CallFunction|Activatesucker))))))
    (:then_1
      (if (CallFunction|TimerPos (Variables|Default|GetCurrentLifeTime) (Variables|Default|GetLifeTimeMax) 1.0 false)
        (Actor|DestroyActor)))))

(fn ConstructionScript)

(fn ActiveSucker
  (params (SetActive :type Boolean)))

(fn Initialize
  (params (ScaleMultiplier :type Float%20%28double-precision%29))
  (CallFunction|ChangeScale ScaleMultiplier))

(fn ChangeScale
  (params (ScaleMultiplier :type Float%20%28double-precision%29))
  (Transformation|SetActorScale3D (* (Class|KismetMathLibrary|VectorOne) ScaleMultiplier)))