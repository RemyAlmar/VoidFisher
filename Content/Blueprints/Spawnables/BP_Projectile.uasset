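; Base spawnable projectile that can start dormant, switch to an active state and destroy itself when its lifetime ends.
; Tick runs both timers; in two-time mode, the trigger timer fires ActivationProjectile once.
; Activation state is passed to ActiveProjectile, an empty function here, with debug prints on spawn and activation.
; Initialize scales Power and actor size by supplied multipliers, using a by-ref helper for the stat.
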(event Custom|ActivationProjectile
  (if (not (Variables|Time|LifeTime|GetbActiveProjectile))
    (bind _output_get (Variables|Time|LifeTime|SetbActiveProjectile true))
    (Public|ActiveProjectile _output_get)
    (Development|PrintString "Activation Projectile" true true "(R=0.044169,G=1.000000,B=0.000000,A=1.000000)" 5.0)))

(event EventBeginPlay
  (Public|ActiveProjectile (Variables|Time|LifeTime|GetbActiveProjectile))
  (Development|PrintString "Apparition Projectile"))

(event EventTick
  (params (DeltaSeconds :type Float%20%28single-precision%29))
  (Utilities|FlowControl|Sequence
    (:then_0
      (if (Variables|Time|TriggerTime|GetIsTwoTimeProjectile)
        (if (not (Variables|Time|LifeTime|GetbActiveProjectile))
          (if (CallFunction|TimerPos (Variables|Time|TriggerTime|GetTriggerTimeCurrent) (Variables|Time|TriggerTime|GetTriggerTimeMax) 1.0 false)
            (Utilities|FlowControl|DoOnce false
              (:Completed
                (CallFunction|ActivationProjectile)))))))
    (:then_1
      (if (CallFunction|TimerPos (Variables|Time|LifeTime|GetCurrentLifeTime) (Variables|Time|LifeTime|GetLifeTimeMax) 1.0 false)
        (Actor|DestroyActor)))))

(fn ConstructionScript)

(fn ActiveProjectile
  (params (SetActive :type Boolean)))

(fn Initialize
  (params (PowerMultiplier :type Float%20%28double-precision%29) (ScaleMultiplier :type Float%20%28single-precision%29))
  (Public|ModifyStat|ChangeFloatStat (Variables|Stat|GetPower) PowerMultiplier)
  (Public|ModifyStat|ChangeScale ScaleMultiplier))

(fn ChangeScale
  (params (ScaleMultiplier :type Float%20%28double-precision%29))
  (Transformation|SetActorScale3D (* (Transformation|GetActorScale3D) ScaleMultiplier)))

(fn ChangeFloatStat
  (params (RefValue :type Float%20%28double-precision%29%20%28by%20ref%29) (Multiplier :type Float%20%28double-precision%29))
  (|SetBy-RefVar RefValue (* RefValue Multiplier)))