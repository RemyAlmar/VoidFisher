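; Spawnable black hole that starts as a physics-simulated capsule, then turns into a stationary gravity source.
; After a trigger timer, activation stops physics, swaps the capsule for the black hole visual and enables BPGravity ticking.
; A separate lifetime timer destroys the actor.
; BPGravity takes its influence and stop spheres at construction; Initialize scales the whole actor and sets gravity force, leaving the radius-change call unwired.
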(event Custom|ActivateBlackHole
  (if (not (Variables|Default|GetbActiveBlackHole))
    (bind _output_get (Variables|Default|SetbActiveBlackHole true))
    (CallFunction|ActiveBlackHole _output_get)
    (Development|PrintString "ActivationBlackHoleSelf" true true "(R=0.044169,G=1.000000,B=0.000000,A=1.000000)" 5.0)))

(event EventBeginPlay
  (CallFunction|ActiveBlackHole (Variables|Default|GetbActiveBlackHole))
  (Development|PrintString "Apparition Trou Noir"))

(event EventTick
  (params (DeltaSeconds :type Float%20%28single-precision%29))
  (Utilities|FlowControl|Sequence
    (:then_0
      (if (not (Variables|Default|GetbActiveBlackHole))
        (if (CallFunction|TimerPos (Variables|Default|GetTriggerTimeCurrent) (Variables|Default|GetTriggerTimeMax) 1.0 false)
          (Utilities|FlowControl|DoOnce false
            (:Completed
              (CallFunction|ActivateBlackHole))))))
    (:then_1
      (if (CallFunction|TimerPos (Variables|Default|GetCurrentLifeTime) (Variables|Default|GetLifeTimeMax) 1.0 false)
        (Actor|DestroyActor)))))

(fn ConstructionScript
  (Default|SetInfluenceSphere (Variables|Default|GetBP_Gravity) (Variables|Default|GetInfluenceOverlap) (Variables|Default|GetStopInfluence)))

(fn ActiveBlackHole
  (params (SetActive :type Boolean))
  (bind _returnvalue (not SetActive))
  (bind _influenceoverlap (Variables|Default|GetInfluenceOverlap))
  (Physics|SetPhysicsLinearVelocity _influenceoverlap "0, 0, 0" false "None")
  (Physics|SetSimulatePhysics _influenceoverlap (not SetActive))
  (Rendering|SetVisibility (Variables|Default|GetCapsule) _returnvalue _returnvalue)
  (Rendering|SetVisibility (Variables|Default|GetBlackHole) SetActive SetActive)
  (Components|Tick|SetComponentTickEnabled (Variables|Default|GetBP_Gravity) SetActive))

(fn ChangeGlobalRadius
  (params (Multiplier :type Float%20%28single-precision%29))
  (Default|ChangeAtmosphereRadius (Variables|Default|GetBP_Gravity) (* (Variables|/Script/Engine.SphereComponent|GetSphereRadius (Variables|Default|GetInfluenceOverlap)) Multiplier))
  (Default|ChangeGroundRadius (Variables|Default|GetBP_Gravity) (* (Variables|/Script/Engine.SphereComponent|GetSphereRadius (Variables|Default|GetStopInfluence)) Multiplier)))

(fn ChangeGravityPower
  (params (AtmosphereGravityForce :type Float%20%28double-precision%29))
  (Variables|/Game/Blueprints/Components/BP_Gravity.BP_Gravity_C|SetAtmosphereGravityForce (Variables|Default|GetBP_Gravity) AtmosphereGravityForce))

(fn GetCurrentGravityPower
  (return (Variables|/Game/Blueprints/Components/BP_Gravity.BP_Gravity_C|GetAtmosphereGravityForce (Variables|Default|GetBP_Gravity))))

(fn Initialize
  (params (RadiusMultiplier :type Float%20%28single-precision%29) (AtmosphereGravityForce :type Float%20%28double-precision%29))
  (CallFunction|ChangeScale RadiusMultiplier)
  (CallFunction|ChangeGravityPower AtmosphereGravityForce))

(fn ChangeScale
  (params (ScaleMultiplier :type Float%20%28double-precision%29))
  (Transformation|SetActorScale3D (* (Class|KismetMathLibrary|VectorOne) ScaleMultiplier)))