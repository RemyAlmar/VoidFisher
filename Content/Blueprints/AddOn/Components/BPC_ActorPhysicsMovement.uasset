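; Actor component that steers and moves a physics-simulated root primitive by setting its linear velocity and rotation directly.
; Self-propulsion and accumulated external forces are interpolated separately, then summed into velocity, with external inputs cleared after each apply.
; Added directions steer a smoothed facing rotation, combined with extra external rotation.
; Helpers cover obstacle traces, cone-based random redirection, impact speed and bounce direction, visual banking roll, and physics toggling.
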(event EventBeginPlay
  (bind _returnvalue (Components|GetOwner))
  (bind _asprimitive_component (Utilities|Casting|CastToPrimitiveComponent (Variables|/Script/Engine.Actor|GetRootComponent _returnvalue))
    (:then
      (Variables|Default|SetOwnRootPhysics _asprimitive_component)
      (Variables|Physics|Forces|Direction|SetTargetDirection (Math|Vector|GetForwardVector (Variables|Default|GetOwnRootPhysics))))
    (:CastFailed
      (Development|PrintText (Utilities|Text|FormatText "{n} not physiqued" (Utilities|GetDisplayName _returnvalue))))))

(fn SetMovementDirection
  (params (Direction :type Vector))
  (Variables|Physics|Forces|Movement|SetTargetSelfForce (* (Variables|Physics|Forces|Speed|GetTargetSpeed) Direction))
  (return))

(fn ApplyMovement
  (params (Direction :type Vector))
  (Movement|SetMovementDirection Direction)
  (Variables|Physics|Forces|Movement|SetSelfForce (Math|Interpolation|VInterpTo (Variables|Physics|Forces|Movement|GetSelfForce) (Variables|Physics|Forces|Movement|GetTargetSelfForce) (Utilities|Time|GetWorldDeltaSeconds) (Variables|Physics|Forces|Speed|Interp|GetInterp%20SpeedSelf)))
  (Variables|Physics|Forces|Movement|SetOtherForces (Math|Interpolation|VInterpTo (Variables|Physics|Forces|Movement|GetOtherForces) (Variables|Physics|Forces|Movement|GetTargetOtherForces) (Utilities|Time|GetWorldDeltaSeconds) (Variables|Physics|Forces|Speed|Interp|GetInterp%20SpeedOtherForce)))
  (Physics|SetPhysicsLinearVelocity (Variables|Default|GetOwnRootPhysics) (+ (Variables|Physics|Forces|Movement|GetSelfForce) (Variables|Physics|Forces|Movement|GetOtherForces)) false "None")
  (Variables|Physics|Forces|Movement|SetTargetOtherForces "0, 0, 0")
  (return))

(fn SetOtherForcesMovement
  (params (OtherForces :type Vector))
  (bind _targetotherforces (Variables|Physics|Forces|Movement|GetTargetOtherForces))
  (|SetBy-RefVar _targetotherforces (+ OtherForces _targetotherforces)))

(fn ChangeDirectiontoRotation
  (Variables|Physics|Forces|Direction|SetTargetDirection (+ (Variables|Physics|Forces|Direction|GetTargetDirection) (Variables|Physics|Forces|Direction|GetAdditiveDirection)))
  (bind (_currentrota _targetrota) (CallFunction|AlignVectors (Variables|Default|GetOwnRootPhysics) (Math|Vector|Normalize (Variables|Physics|Forces|Direction|GetTargetDirection))))
  (bind _returnvalue (CallFunction|AlignSmooth _currentrota _targetrota (Variables|Physics|Rotation|GetRotationRate)))
  (Variables|Physics|Rotation|SetTargetSelfRotation _returnvalue)
  (Variables|Physics|Forces|Direction|SetAdditiveDirection "0, 0, 0")
  (return))

(fn SetRandomDirection
  (params (ConeAngle :type Float%20%28double-precision%29) (Range :type Float%20%28double-precision%29) (RadiusToCover :type Integer))
  (bind _returnvalue (Components|GetOwner))
  (bind (_output _hasadirection) (CallFunction|GetOneDirectionfromSphereRadius 6 (Transformation|GetActorLocation _returnvalue) (Transformation|GetActorForwardVector _returnvalue) ConeAngle Range RadiusToCover "TraceTypeQuery1" "None" 2.0 "(R=0.000000,G=0.846483,B=1.000000,A=1.000000)"))
  (if _hasadirection
    (CallFunction|AddDirection _output))
  (return))

(fn CanMovetoCurrentDirection
  (params (Range :type Float%20%28double-precision%29))
  (bind _returnvalue (Components|GetOwner))
  (bind _returnvalue_2 (Transformation|GetActorLocation _returnvalue))
  (bind _returnvalue_3 (Collision|LineTraceByChannel _returnvalue_2 (+ _returnvalue_2 (* Range (Transformation|GetActorForwardVector _returnvalue))) "TraceTypeQuery3" true 0 "None" true "(R=0.000000,G=0.623424,B=1.000000,A=1.000000)" "(R=1.000000,G=0.151168,B=0.000000,A=1.000000)" 0.0))
  (return (not _returnvalue_3)))

(fn SetOtherRotation
  (params (OtherRota :type Rotator))
  (bind _targetotherrotation (Variables|Physics|Rotation|GetTargetOtherRotation))
  (|SetBy-RefVar _targetotherrotation (Class|KismetMathLibrary|QuatRotator (* (Math|Conversions|ToQuaternion(Rotator) _targetotherrotation) (Class|KismetMathLibrary|QuatNormalized (Math|Conversions|ToQuaternion(Rotator) OtherRota) 0.0001))))
  (return))

(fn ApplyRotation
  (Rotation|ChangeDirectiontoRotation)
  (Transformation|SetWorldRotation (Variables|Default|GetOwnRootPhysics) (Variables|Physics|Rotation|GetTargetSelfRotation) false false)
  (Transformation|AddWorldRotation (Variables|Default|GetOwnRootPhysics) (Variables|Physics|Rotation|GetTargetOtherRotation) false false)
  (Variables|Physics|Rotation|SetTargetOtherRotation "0, 0, 0")
  (return))

(fn SetRollonSceneComp
  (params (Target :type Scene%20Component%20Object%20Reference%20%28by%20ref%29) (AngleMaxToRoll :type Float%20%28double-precision%29) (InterpSpeed :type Float%20%28single-precision%29))
  (bind _ownrootphysics (Variables|Default|GetOwnRootPhysics))
  (LocalVariables|SetAnglePower (Math|Float|NormalizetoRange (CallFunction|GetSideBetween2Vec (Math|Vector|GetForwardVector _ownrootphysics) (Math|Vector|Normalize (Variables|Physics|Forces|Direction|GetTargetDirection)) (Math|Vector|GetUpVector _ownrootphysics)) 0.0 0.1))
  (Transformation|SetRelativeRotation Target (Math|Interpolation|RInterpTo (Variables|/Script/Engine.SceneComponent|GetRelativeRotation Target) (Math|Rotator|MakeRotator (* (LocalVariables|GetAnglePower) AngleMaxToRoll) 0.0 0.0) (Utilities|Time|GetWorldDeltaSeconds) InterpSpeed) false false)
  (return))

(fn GetSpeed
  (return (Math|Vector|VectorLength (CallFunction|GetVelocity (Variables|Default|GetOwnRootPhysics)))))

(fn ChangeSpeedonImpact
  (params (ImpactNormalDirection :type Vector))
  (bind _selfforce (Variables|Physics|Forces|Movement|GetSelfForce))
  (bind _returnvalue (Math|Vector|VectorLength _selfforce))
  (Variables|Physics|Forces|Speed|SetTargetSpeed (+ (* _returnvalue (Math|Vector|DotProduct ImpactNormalDirection (Math|Vector|GetForwardVector (Variables|Default|GetOwnRootPhysics)))) _returnvalue))
  (return))

(fn GetBoundDirection
  (params (ImpactNormal :type Vector))
  (return (Math|Vector|Normalize (* (- (CallFunction|GetVelocity (Variables|Default|GetOwnRootPhysics)) (* (* (Math|Vector|DotProduct (Math|Vector|GetForwardVector (Variables|Default|GetOwnRootPhysics)) ImpactNormal) ImpactNormal) 2.0)) (Math|Vector|VectorLength (Variables|Physics|Forces|Movement|GetSelfForce))))))

(fn On/OffPhysics
  (params (Active :type Boolean) (CurrentSpeed :type Float%20%28double-precision%29))
  (Variables|Physics|Forces|Speed|SetTargetSpeed CurrentSpeed)
  (Physics|SetSimulatePhysics (Variables|Default|GetOwnRootPhysics) Active))

(fn StopSpeed
  (Variables|Physics|Forces|Speed|SetTargetSpeed 0.0)
  (Variables|Physics|Forces|Movement|SetSelfForce "0, 0, 0")
  (Variables|Physics|Forces|Movement|SetTargetSelfForce "0, 0, 0")
  (return))

(fn GetDirection
  (bind _ownrootphysics (Variables|Default|GetOwnRootPhysics))
  (return (Math|Vector|DotProduct (Math|Vector|GetForwardVector _ownrootphysics) (Math|Vector|Normalize (CallFunction|GetVelocity _ownrootphysics)))))

(fn AddDirection
  (params (DirectionAdditive :type Vector))
  (Variables|Physics|Forces|Direction|SetAdditiveDirection (+ (Variables|Physics|Forces|Direction|GetAdditiveDirection) DirectionAdditive)))