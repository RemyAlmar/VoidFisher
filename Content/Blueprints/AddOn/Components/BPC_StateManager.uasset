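; BPC_StateManager is an actor component that gives its owner a state machine, delegating to a BP_StateCommander created on BeginPlay.
; Initialize hands the owner and a class map to the commander, and IUpdate forwards ticks to it.
; AddState constructs and registers states at runtime, skipping classes already listed in the map and occupied enum slots, and can switch immediately.
; Component activation re-enters the current state, if any exists.
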(event Custom|ED_OnComponentActivated_Event
  (params (Component :type Actor%20Component%20Object%20Reference) (bReset :type Boolean))
  (CallFunction|RestartState))

(event Custom|RestartState
  (bind _statecommander (Variables|Default|GetStateCommander))
  (if (Default|HasAnyState _statecommander)
    (Default|IChangeState _statecommander (Default|GetCurrentStateByte _statecommander))))

(event Custom|ED_OnComponentDeactivate_Event
  (params (Component :type Actor%20Component%20Object%20Reference)))

(event EventBeginPlay
  (bind _returnvalue (Game|ConstructObjectfromClass "/Game/Blueprints/AI/StateMachine/BP_StateCommander.BP_StateCommander_C"))
  (Variables|Default|SetStateCommander _returnvalue)
  (Components|Activation|BindEventtoOnComponentActivated (EventDispatchers|CreateEvent :!event Custom|ED_OnComponentActivated_Event))
  (EventDispatchers|BindEventtoOnComponentDeactivated (EventDispatchers|CreateEvent :!event Custom|ED_OnComponentDeactivate_Event)))

(event EventIUpdate
  (params (DeltaSeconds :type Float%20%28double-precision%29))
  (Default|IUpdate (Variables|Default|GetStateCommander) DeltaSeconds))

(fn Initialize
  (params (List%20States%20Class :type Map%20of%20Bytes%20to%20Structs))
  (bind _output_get (Variables|Default|SetList%20States%20Class List%20States%20Class))
  (Default|InititalizeCommander (Variables|Default|GetStateCommander) (Components|GetOwner) _output_get))

(fn AddState
  (params (TargetEnum :type Byte) (StartThisState :type Boolean) (ClassState :type BP%20State%20Class%20Reference))
  (bind (_targetenum _returnvalue) (CallFunction|HasClassInstancied ClassState))
  (LocalVariables|SetLocalTargetEnum TargetEnum)
  (if _returnvalue
    (LocalVariables|SetLocalTargetEnum _targetenum)
    (elif (Default|HasState (Variables|Default|GetStateCommander) (LocalVariables|GetLocalTargetEnum))
      _
      (else
        (bind _returnvalue_2 (Game|ConstructObjectfromClass ClassState))
        (bind _output_get (LocalVariables|SetLocalState _returnvalue_2))
        (Default|InitState _output_get (Components|GetOwner) TargetEnum (Variables|Default|GetStateCommander))
        (Default|AddState (Variables|Default|GetStateCommander) TargetEnum (LocalVariables|GetLocalState)))))
  (if StartThisState
    (Default|IChangeState (Variables|Default|GetStateCommander) TargetEnum)
    (return)))

(fn HasClassInstancied
  (params (TargetClass :type Object%20Class%20Reference))
  (bind _values (Utilities|Map|Values (Variables|Default|GetList%20States%20Class)))
  (for (_array_element _array_index) _values
    (if (== (Utilities|Struct|BreakS_StateCooldown _array_element) TargetClass)
      (LocalVariables|SetTargetClassExist (== (Utilities|Struct|BreakS_StateCooldown _array_element) TargetClass))
      (bind _keys (Utilities|Map|Keys (Variables|Default|GetList%20States%20Class)))
      (return (Utilities|Array|Get(acopy) _keys _array_index) (LocalVariables|GetTargetClassExist))))
  (return (Utilities|Array|Get(acopy) _keys _array_index) (LocalVariables|GetTargetClassExist)))