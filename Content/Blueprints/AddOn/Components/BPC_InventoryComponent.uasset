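; Inventory component that stores caught or collected creatures in a map keyed by creature name.
; AddData inserts a new entry or, for an existing creature, merges stats by summing Quantity and keeping the larger Size and Weight while retaining other fields.
; AddData and ClearData both push the updated map to the owning actor through UpdateDataMessage.
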(event EventClearData
  (bind _items (Variables|Default|GetItems))
  (Utilities|Map|Clear _items)
  (Class|BPIInventory|UpdateData(Message) (Components|GetOwner) _items))

(event EventAddData
  (params (Data :type S%20Creature%20Details%20Instanced%20Structure))
  (bind _mapvalue (CallFunction|AddInventory (Variables|Default|GetItems) Data))
  (Class|BPIInventory|UpdateData(Message) (Components|GetOwner) _mapvalue))

(fn ModifySettings
  (params (TargetMap :type Map%20of%20E_CreatureType%20Enums%20to%20Structs :default "NewEnumerator4") (CreatureType :type E_CreatureType%20Enum%20%28by%20ref%29 :default "NewEnumerator4") (Creature%20Stat%20Settings :type S%20AI%20Creature%20Stat%20Settings%20Structure))
  (bind _items (Variables|Default|GetItems))
  (bind _value (Utilities|Map|Find _items CreatureType))
  (bind (_creaturemesh _animblueprint _staticmesh _material _size _weight _quantity _xp) (Utilities|Struct|BreakS_AICreatureStatSettings (.creaturestatsettings _value)))
  (Utilities|Map|Add TargetMap CreatureType (Utilities|Struct|MakeS_CreatureDetailsInstanced (.creaturename _value) (.creaturesizetype _value) (.creaturedescription _value) (Utilities|Struct|MakeS_AICreatureStatSettings _creaturemesh _animblueprint _staticmesh 0 (Math|Float|Max(Float) _size (.size Creature%20Stat%20Settings)) (Math|Float|Max(Float) _weight (.weight Creature%20Stat%20Settings)) (+ _quantity (.quantity Creature%20Stat%20Settings)) _xp) (.creaturebehaviorsettings _value)))
  (return))

(fn AddInventory
  (params (TargetMap :type Map%20of%20E_CreatureType%20Enums%20to%20Structs :default "NewEnumerator4") (CreatureDetailsInstanced :type S%20Creature%20Details%20Instanced%20Structure%20%28by%20ref%29))
  (bind (_creaturename _creaturestatsettings) (Utilities|Struct|BreakS_CreatureDetailsInstanced CreatureDetailsInstanced))
  (if (.ReturnValue (Utilities|Map|Find TargetMap _creaturename))
    (CallFunction|ModifySettings TargetMap _creaturename _creaturestatsettings)
    (else
      (Utilities|Map|Add TargetMap _creaturename CreatureDetailsInstanced)))
  (return TargetMap))