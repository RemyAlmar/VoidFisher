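; Component that manages the ship's tools, tracking the active one and handling open, close, toggle, use, unlock and upgrade.
; Tools live in an enum-keyed map, and the manager forwards actions to each tool, then broadcasts matching event dispatchers.
; Toggling switches tools, or closes the current one if the requested tool is locked or already active.
; Helpers check unlock eligibility by player level and zone, and upgrade eligibility by tool level.
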(fn OpenTool
  (params (ToolToOpen :type E_ToolShip%20Enum :default "NewEnumerator0"))
  (bind _toollist (Variables|Default|GetToolList))
  (bind (_value _returnvalue) (Utilities|Map|Find _toollist ToolToOpen))
  (if _returnvalue
    (Default|CallEDActiveTool _value)
    (bind _output_get (Variables|Default|SetCurrentToolActive ToolToOpen))
    (Default|CallEDonActiveToolManager _output_get)
    (else
      (Development|PrintText (Utilities|Text|FormatText "WARNING : Tool Missing {name}" (Utilities|String|EnumtoString ToolToOpen)) true true "(R=1.000000,G=0.587717,B=0.000000,A=1.000000)" 5.0))))

(fn CloseTool
  (params (ToolToClosed :type E_ToolShip%20Enum :default "NewEnumerator0"))
  (bind _toollist (Variables|Default|GetToolList))
  (bind (_value _returnvalue) (Utilities|Map|Find _toollist ToolToClosed))
  (if _returnvalue
    (Default|CallEDDeactiveTool _value)
    (Default|CallEDonDeactiveToolManager ToolToClosed)
    (Variables|Default|SetCurrentToolActive "NewEnumerator3")))

(fn UnlockTool
  (params (ToolToUnlock :type E_ToolShip%20Enum :default "NewEnumerator3"))
  (bind _toollist (Variables|Default|GetToolList))
  (bind (_value _returnvalue) (Utilities|Map|Find _toollist ToolToUnlock))
  (if _returnvalue
    (Default|CallEDUnlockTool _value)
    (Default|CallEDonUnlockToolManager ToolToUnlock)
    (else
      (Development|PrintText (Utilities|Text|FormatText "{name} don't exist in tool manager" (Utilities|String|EnumtoString ToolToUnlock))))))

(fn UseTool
  (bind _toollist (Variables|Default|GetToolList))
  (bind _currenttoolactive (Variables|Default|GetCurrentToolActive))
  (bind (_value _returnvalue) (Utilities|Map|Find _toollist _currenttoolactive))
  (if _returnvalue
    (Default|CallEDUseTool _value)
    (Default|CallEDonUseToolManager (Variables|Default|GetCurrentToolActive))))

(fn UseSecondaryTool
  (bind _toollist (Variables|Default|GetToolList))
  (bind _currenttoolactive (Variables|Default|GetCurrentToolActive))
  (bind (_value _returnvalue) (Utilities|Map|Find _toollist _currenttoolactive))
  (if _returnvalue
    (Default|CallEDUseToolSecondaryMode _value)
    (Default|CallEDonUseSecondaryToolManager (Variables|Default|GetCurrentToolActive))))

(fn ToggleTool
  (params (NextTool :type E_ToolShip%20Enum :default "NewEnumerator3"))
  (if (Public|ToolLock|IsLock NextTool)
    (Private|CloseTool (Variables|Default|GetCurrentToolActive) :!label _label)
    (Audio|PlaySound2D (Variables|Default|GetDeactiveTool_SFX) 1.0 1.0 0.0 0 0)
    (elif (Private|AlreadyActive NextTool)
      (goto _label)
      (else
        (Private|SwitchTool NextTool)))))

(fn SwitchTool
  (params (NewTool :type E_ToolShip%20Enum :default "NewEnumerator0"))
  (Private|CloseTool (Variables|Default|GetCurrentToolActive))
  (Private|OpenTool NewTool))

(fn AlreadyActive
  (params (ToolToActive :type E_ToolShip%20Enum :default "NewEnumerator3"))
  (return (Utilities|Enum|Equal(Enum) ToolToActive (Variables|Default|GetCurrentToolActive))))

(fn AddTool
  (params (Key :type E_ToolShip%20Enum%20%28by%20ref%29 :default "NewEnumerator3") (Value :type BPC%20Tool%20Base%20Object%20Reference%20%28by%20ref%29))
  (Utilities|Map|Add (Variables|Default|GetToolList) Key Value)
  (Default|Initialize Value))

(fn IsLock
  (params (Tool :type E_ToolShip%20Enum%20%28by%20ref%29 :default "NewEnumerator3"))
  (bind _toollist (Variables|Default|GetToolList))
  (bind (_value _returnvalue) (Utilities|Map|Find _toollist Tool))
  (if _returnvalue
    (return (Variables|/Game/Blueprints/Game/Player/ToolsComponent/BPC_ToolBase.BPC_ToolBase_C|GetIsLock _value))))

(fn GetCurrentLevel
  (params (Tool :type E_ToolShip%20Enum :default "NewEnumerator3"))
  (bind _toollist (Variables|Default|GetToolList))
  (bind (_value _returnvalue) (Utilities|Map|Find _toollist Tool))
  (if _returnvalue
    (return (Variables|/Game/Blueprints/Game/Player/ToolsComponent/BPC_ToolBase.BPC_ToolBase_C|GetCurrentLevel _value))))

(fn GetNextLevel
  (params (Tool :type E_ToolShip%20Enum :default "NewEnumerator3") (NextValue :type Integer))
  (bind _toollist (Variables|Default|GetToolList))
  (bind (_value _returnvalue) (Utilities|Map|Find _toollist Tool))
  (if _returnvalue
    (return (Variables|/Game/Blueprints/Game/Player/ToolsComponent/BPC_ToolBase.BPC_ToolBase_C|GetCurrentLevel _value))))

(fn UpgradeTool
  (params (ToolToUpgrade :type E_ToolShip%20Enum :default "NewEnumerator3"))
  (Default|ToolBaseEDUpgradeNextLevel (.Value (Utilities|Map|Find (Variables|Default|GetToolList) ToolToUpgrade)))
  (Default|CallEDonUpgradeToolManager ToolToUpgrade))

(fn GetTotalLevel
  (params (Tool :type E_ToolShip%20Enum :default "NewEnumerator3"))
  (bind _returnvalue (Default|GetTotalLevel (.Value (Utilities|Map|Find (Variables|Default|GetToolList) Tool))))
  (return _returnvalue))

(fn CanbeDelock
  (params (Tool :type E_ToolShip%20Enum :default "NewEnumerator3") (PlayerLevel :type Integer) (Current%20Zone%20Delock :type Array%20of%20E_Levels%20Enums :default "NewEnumerator0"))
  (bind _toollist (Variables|Default|GetToolList))
  (bind (_value _returnvalue) (Utilities|Map|Find _toollist Tool))
  (if _returnvalue
    (bind (_stat_name _level_needed _zone_needed) (Default|GetData _value))
    (if (>= PlayerLevel _level_needed) ; a le level
      (if (Utilities|Array|ContainsItem Current%20Zone%20Delock _zone_needed) ; A delock la zone
        (return true) ; Peut être delock
        (else
          _)))
    (else
      (Development|PrintString "Tool No Valid For Unlock" true true "(R=1.000000,G=0.000000,B=0.101925,A=1.000000)" 5.0)))
  (return false) ; Ne peut pas
)

(fn CanbeUpgrade
  (params (Tool :type E_ToolShip%20Enum :default "NewEnumerator3"))
  (bind _currentlevel (Public|ToolLevel|GetCurrentLevel Tool))
  (if (.ReturnValue (Utilities|Map|Find (Variables|Default|GetToolList) Tool))
    (if (Public|ToolLock|IsLock Tool)
      (return false)
      (else
        (Math|Integer|IncrementInt _currentlevel
          (:%20%20
            (if (>= _currentlevel (Public|ToolLevel|GetTotalLevel Tool))
              (return false)
              (else
                _))))))
    (else
      (Development|PrintString "Le tool n'existe pas " true true "(R=1.000000,G=0.000000,B=0.018869,A=1.000000)" 1e+01)))
  (return true))

(fn AddTool
  (params (Key :type E_ToolShip%20Enum%20%28by%20ref%29 :default "NewEnumerator3") (Value :type BPC%20Tool%20Base%20Object%20Reference%20%28by%20ref%29))
  (Utilities|Map|Add (Variables|Default|GetToolList) Key Value)
  (Default|Initialize Value))

(fn AlreadyActive
  (params (ToolToActive :type E_ToolShip%20Enum :default "NewEnumerator3"))
  (return (Utilities|Enum|Equal(Enum) ToolToActive (Variables|Default|GetCurrentToolActive))))

(fn CloseTool
  (params (ToolToClosed :type E_ToolShip%20Enum :default "NewEnumerator0"))
  (bind _toollist (Variables|Default|GetToolList))
  (bind (_value _returnvalue) (Utilities|Map|Find _toollist ToolToClosed))
  (if _returnvalue
    (Default|CallEDDeactiveTool _value)
    (Default|CallEDonDeactiveToolManager ToolToClosed)
    (Variables|Default|SetCurrentToolActive "NewEnumerator3")))

(fn EDonActiveToolManager
  (params (CurrentTool :type E_ToolShip%20Enum :default "NewEnumerator3")))

(fn EDonDeactiveToolManager
  (params (CurrentTool :type E_ToolShip%20Enum :default "NewEnumerator3")))

(fn EDonUnlockToolManager
  (params (ToolUnlocked :type E_ToolShip%20Enum :default "NewEnumerator3")))

(fn EDonUpgradeToolManager
  (params (CurrentTool :type E_ToolShip%20Enum :default "NewEnumerator3")))

(fn EDonUseSecondaryToolManager
  (params (CurrentTool :type E_ToolShip%20Enum :default "NewEnumerator3")))

(fn EDonUseToolManager
  (params (CurrentTool :type E_ToolShip%20Enum :default "NewEnumerator3")))

(fn GetCurrentLevel
  (params (Tool :type E_ToolShip%20Enum :default "NewEnumerator3"))
  (bind _toollist (Variables|Default|GetToolList))
  (bind (_value _returnvalue) (Utilities|Map|Find _toollist Tool))
  (if _returnvalue
    (return (Variables|/Game/Blueprints/Game/Player/ToolsComponent/BPC_ToolBase.BPC_ToolBase_C|GetCurrentLevel _value))))

(fn GetNextLevel
  (params (Tool :type E_ToolShip%20Enum :default "NewEnumerator3") (NextValue :type Integer))
  (bind _toollist (Variables|Default|GetToolList))
  (bind (_value _returnvalue) (Utilities|Map|Find _toollist Tool))
  (if _returnvalue
    (return (Variables|/Game/Blueprints/Game/Player/ToolsComponent/BPC_ToolBase.BPC_ToolBase_C|GetCurrentLevel _value))))

(fn IsLock
  (params (Tool :type E_ToolShip%20Enum%20%28by%20ref%29 :default "NewEnumerator3"))
  (bind _toollist (Variables|Default|GetToolList))
  (bind (_value _returnvalue) (Utilities|Map|Find _toollist Tool))
  (if _returnvalue
    (return (Variables|/Game/Blueprints/Game/Player/ToolsComponent/BPC_ToolBase.BPC_ToolBase_C|GetIsLock _value))))

(fn OpenTool
  (params (ToolToOpen :type E_ToolShip%20Enum :default "NewEnumerator0"))
  (bind _toollist (Variables|Default|GetToolList))
  (bind (_value _returnvalue) (Utilities|Map|Find _toollist ToolToOpen))
  (if _returnvalue
    (Default|CallEDActiveTool _value)
    (bind _output_get (Variables|Default|SetCurrentToolActive ToolToOpen))
    (Default|CallEDonActiveToolManager _output_get)
    (else
      (Development|PrintText (Utilities|Text|FormatText "WARNING : Tool Missing {name}" (Utilities|String|EnumtoString ToolToOpen)) true true "(R=1.000000,G=0.587717,B=0.000000,A=1.000000)" 5.0))))

(fn SwitchTool
  (params (NewTool :type E_ToolShip%20Enum :default "NewEnumerator0"))
  (Private|CloseTool (Variables|Default|GetCurrentToolActive))
  (Private|OpenTool NewTool))

(fn ToggleTool
  (params (NextTool :type E_ToolShip%20Enum :default "NewEnumerator3"))
  (if (Public|ToolLock|IsLock NextTool)
    (Private|CloseTool (Variables|Default|GetCurrentToolActive) :!label _label)
    (elif (Private|AlreadyActive NextTool)
      (goto _label)
      (else
        (Private|SwitchTool NextTool)))))

(fn UnlockTool
  (params (ToolToUnlock :type E_ToolShip%20Enum :default "NewEnumerator3"))
  (Default|CallEDUnlockTool (.Value (Utilities|Map|Find (Variables|Default|GetToolList) ToolToUnlock)))
  (Default|CallEDonUnlockToolManager ToolToUnlock))

(fn UpgradeTool
  (params (ToolToUpgrade :type E_ToolShip%20Enum%20%28by%20ref%29 :default "NewEnumerator3"))
  (Default|ToolBaseEDUpgradeNextLevel (.Value (Utilities|Map|Find (Variables|Default|GetToolList) ToolToUpgrade)))
  (Default|CallEDonUpgradeToolManager ToolToUpgrade))

(fn UseSecondaryTool
  (bind _toollist (Variables|Default|GetToolList))
  (bind _currenttoolactive (Variables|Default|GetCurrentToolActive))
  (bind (_value _returnvalue) (Utilities|Map|Find _toollist _currenttoolactive))
  (if _returnvalue
    (Default|CallEDUseToolSecondaryMode _value)
    (Default|CallEDonUseSecondaryToolManager (Variables|Default|GetCurrentToolActive))))

(fn UseTool
  (bind _toollist (Variables|Default|GetToolList))
  (bind _currenttoolactive (Variables|Default|GetCurrentToolActive))
  (bind (_value _returnvalue) (Utilities|Map|Find _toollist _currenttoolactive))
  (if _returnvalue
    (Default|CallEDUseTool _value)
    (Default|CallEDonUseToolManager (Variables|Default|GetCurrentToolActive))
    (else
      (Audio|PlaySound2D "/Game/SFX/Sounds/OGG/Outils/CUE/SFX_outils-01_Cue.SFX_outils-01_Cue" 1.0 1.0 0.0 0 0))))