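; BPC_VFX_Manager is an actor component that spawns, tracks and tweaks Niagara effects by VFX type.
; Adding a type spawns its template from a lookup map, at a location or attached, and stores one instance per type.
; Attach targets come from a named component map or the owner's skeletal mesh, with sockets picked by name prefix and index.
; Helpers remove effects, set float, color and material parameters, and read materials.
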(fn GetComponenttoAttach
  (params (ComponentName :type String) (SkeletalMeshComponent :type Boolean))
  (LocalVariables|SetCurrentSceneComp (.Value (Utilities|Map|Find (Variables|Default|GetAttachedComponentList) ComponentName)))
  (if SkeletalMeshComponent
    (bind _skeletalmesh (Class|BPIGetData|GetSkeletalMesh(Message) (Components|GetOwner)))
    (LocalVariables|SetSKM_Scene (Utilities|ResolveSoftReference _skeletalmesh))
    (if (== (LocalVariables|GetCurrentSceneComp) (LocalVariables|GetSKM_Scene))
      _
      (else
        (HandleComponents|AddComponenttoAttach "SKM" (LocalVariables|GetSKM_Scene))))
    (LocalVariables|SetCurrentSceneComp (LocalVariables|GetSKM_Scene)))
  (Utilities|IsValid (LocalVariables|GetCurrentSceneComp)
    (:Is%20Valid
      _)
    (:Is%20Not%20Valid
      (bind _values (Utilities|Map|Values (Variables|Default|GetAttachedComponentList)))
      (if (Utilities|Array|IsNotEmpty _values)
        (LocalVariables|SetCurrentSceneComp (Utilities|Array|Get(acopy) _values))
        (else
          (HandleComponents|AddComponenttoAttach "Root" (Variables|/Script/Engine.Actor|GetRootComponent (Components|GetOwner)))))))
  (return (LocalVariables|GetCurrentSceneComp)))

(fn GetNiagaraSystem
  (params (VFXType :type E_VFXType%20Enum%20%28by%20ref%29 :default "NewEnumerator2"))
  (bind _output_get (LocalVariables|SetCurrentNPS (.Value (Utilities|Map|Find (Variables|Default|GetNPS_CompoList) VFXType))))
  (Utilities|IsValid _output_get
    (:Is%20Valid
      (return (LocalVariables|GetCurrentNPS)))
    (:Is%20Not%20Valid
      (Development|PrintText (Utilities|Text|FormatText "VFX_Manager : Niagara System of Type {x} not found" (Utilities|String|EnumtoString VFXType)) true true "(R=1.000000,G=0.000000,B=0.159007,A=1.000000)" 1e+01))))

(fn AddComponenttoAttach
  (params (Name :type String) (Comp :type Scene%20Component%20Object%20Reference))
  (bind _attachedcomponentlist (Variables|Default|GetAttachedComponentList))
  (Utilities|IsValid (.Value (Utilities|Map|Find _attachedcomponentlist Name))
    (:Is%20Valid
      _)
    (:Is%20Not%20Valid
      (Utilities|Map|Add _attachedcomponentlist Name Comp)))
  (return))

(fn RemoveComponenttoAttach
  (params (Name :type String%20%28by%20ref%29))
  (LocalVariables|SetCurrentComp (.Value (Utilities|Map|Find (Variables|Default|GetAttachedComponentList) Name)))
  (Utilities|Map|Remove (Variables|Default|GetAttachedComponentList) Name)
  (Utilities|IsValid (LocalVariables|GetCurrentComp)
    (:Is%20Valid
      (Components|DestroyComponent (LocalVariables|GetCurrentComp)))
    (:Is%20Not%20Valid
      _))
  (return))

(fn SetComponenttoAttach
  (params (Name :type String%20%28by%20ref%29) (Comp :type Scene%20Component%20Object%20Reference))
  (HandleComponents|RemoveComponenttoAttach Name)
  (Utilities|IsValid Comp
    (:Is%20Valid
      (HandleComponents|AddComponenttoAttach Name Comp))))

(fn AddNiagaraSystem
  (params (Type :type E_VFXType%20Enum :default "NewEnumerator1") (HaveToAttached :type Boolean) (Location :type Vector) (Rotation :type Rotator) (Scale :type Vector :default "1.000000,1.000000,1.000000") (bAutoDestroy :type Boolean) (bAutoActivate :type Boolean) (ComponentNameToAttach :type String) (SocketPrefixNameToAttach :type String) (IndexSocket :type Integer) (WantSkeletalMeshComponent :type Boolean))
  (bind _ns_list (Variables|Default|GetNS_List))
  (bind _value (Utilities|Map|Find _ns_list Type))
  (LocalVariables|SetCurHaveToAttached HaveToAttached)
  (if (Utilities|Enum|Equal(Enum) ComponentNameToAttach "")
    (LocalVariables|SetCurHaveToAttached false))
  (Utilities|IsValid (.Value (Utilities|Map|Find (Variables|Default|GetNPS_CompoList) Type))
    (:Is%20Valid
      _)
    (:Is%20Not%20Valid
      (if (LocalVariables|GetCurHaveToAttached)
        (bind _returnvalue (Niagara|SpawnSystemAttached _value (HandleComponents|Getter|GetComponenttoAttach ComponentNameToAttach WantSkeletalMeshComponent) (HandleComponents|Getter|GetSocketfromComp ComponentNameToAttach SocketPrefixNameToAttach IndexSocket WantSkeletalMeshComponent) Location Rotation "KeepRelativeOffset" bAutoDestroy (Variables|Activation|GetbAutoActivate)))
        (LocalVariables|SetCurrentNPS _returnvalue)
        (else
          (bind _returnvalue_2 (Niagara|SpawnSystematLocation _value Location Rotation Scale bAutoDestroy (Variables|Activation|GetbAutoActivate)))
          (LocalVariables|SetCurrentNPS _returnvalue_2)))
      (Utilities|Map|Add (Variables|Default|GetNPS_CompoList) Type (LocalVariables|GetCurrentNPS))))
  (return))

(fn GetSocketfromComp
  (params (CompName :type String%20%28by%20ref%29) (SocketPrefixName :type String) (IndexSocket :type Integer) (FromSkeletalMeshComponent :type Boolean))
  (bind _componentout (HandleComponents|Getter|GetComponenttoAttach CompName FromSkeletalMeshComponent))
  (bind _returnvalue (Transformation|GetAllSocketNames _componentout))
  (bind _outsocketanchorlist (CallFunction|GetSocketName SocketPrefixName _returnvalue))
  (if (Utilities|Array|IsNotEmpty _outsocketanchorlist)
    (LocalVariables|SetCurrentSocketName (Utilities|Array|Get(acopy) _outsocketanchorlist IndexSocket)))
  (return (LocalVariables|GetCurrentSocketName)))

(fn RemoveNiagaraSystem
  (params (Type :type E_VFXType%20Enum :default "NewEnumerator1"))
  (bind _nps_compolist (Variables|Default|GetNPS_CompoList))
  (bind _value (Utilities|Map|Find _nps_compolist Type))
  (LocalVariables|SetCurrentNPS _value)
  (Components|DestroyComponent _value)
  (Utilities|Map|Remove (Variables|Default|GetNPS_CompoList) Type)
  (return))

(fn SetMaterialNiagaraSystem
  (params (Type :type E_VFXType%20Enum :default "NewEnumerator1") (ParameterName :type Name :default "Material") (Material :type Material%20Interface%20Object%20Reference))
  (Class|NiagaraComponent|SetVariableMaterial (HandleNiagaraSystem|Getter|GetNiagaraSystem Type) ParameterName Material)
  (return))

(fn SetFloatNiagaraSystem
  (params (Type :type E_VFXType%20Enum :default "NewEnumerator1") (ParameterName :type Name :default "Material") (Value :type Float%20%28double-precision%29))
  (Niagara|SetNiagaraVariable(Float) (HandleNiagaraSystem|Getter|GetNiagaraSystem Type) ParameterName Value)
  (return))

(fn SetColorNiagaraSystem
  (params (Type :type E_VFXType%20Enum :default "NewEnumerator1") (ParameterName :type Name :default "Material") (ColorValue :type Linear%20Color%20Structure :default "(R=1.000000,G=1.000000,B=1.000000,A=1.000000)"))
  (Niagara|SetNiagaraVariable(LinearColor) (HandleNiagaraSystem|Getter|GetNiagaraSystem Type) ParameterName ColorValue)
  (return))

(fn GetMaterialNiagaraSystem
  (params (Type :type E_VFXType%20Enum :default "NewEnumerator1") (Index :type Integer))
  (return (Rendering|Material|GetMaterial (HandleNiagaraSystem|Getter|GetNiagaraSystem Type) Index)))