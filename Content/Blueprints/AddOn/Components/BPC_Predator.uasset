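; Predator actor component that lets its owner detect and hunt smaller actors carrying a BPC_Prey component.
; Overlaps on an injected detection component fill an in-range list, which Tick filters by distance into a hunt list.
; It keeps a valid current prey or picks a replacement by distance, registers itself on that prey and fires hunt dispatchers.
; Helpers expose prey direction, proximity and line-trace visibility, though the hunt logic shown skips the visibility check.
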(event Custom|OnBeginOverlap
  (params (OverlappedComponent :type Primitive%20Component%20Object%20Reference) (OtherActor :type Actor%20Object%20Reference) (OtherComp :type Primitive%20Component%20Object%20Reference) (OtherBodyIndex :type Integer) (bFromSweep :type Boolean) (SweepResult :type Hit%20Result%20Structure%20%28by%20ref%29))
  (bind _returnvalue (Actor|GetComponentbyClass OtherActor "/Game/Blueprints/AddOn/Components/BPC_Prey.BPC_Prey_C"))
  (Utilities|IsValid _returnvalue
    (:Is%20Valid
      (if (CallFunction|IsAPrey (Variables|/Game/Blueprints/AddOn/Components/BPC_Prey.BPC_Prey_C|GetSizeSelf _returnvalue))
        (CallFunction|AddPreyinRangeEvent OtherActor)))))

(event Custom|Event_RemovePreyToHunt_Event
  (params (PreyToRemoveFromHunt :type Actor%20Object%20Reference))
  ;[1 0.2033 0] Chasse les proies visible
  (if (Utilities|Array|ContainsItem (Variables|Default|GetActorsInSight) PreyToRemoveFromHunt)
    (Utilities|Array|RemoveItem (Variables|Default|GetActorsInSight) PreyToRemoveFromHunt)
    (Default|CallEDRemovePreytoHunt PreyToRemoveFromHunt)
    (if (Utilities|Array|IsEmpty (Variables|Default|GetActorsInSight))
      (Default|CallEDIsWithoutPrey)
      (Variables|Default|SetCurrentPrey 0)
      (else
        (CallFunction|ChangePrey)))))

(event Custom|ChangePrey
  (bind _currentprey (Variables|Default|GetCurrentPrey)
    (:then
      (Utilities|IsValid (Actor|GetComponentbyClass _currentprey "/Game/Blueprints/AddOn/Components/BPC_Prey.BPC_Prey_C")
        (:Is%20Valid
          (Default|RemoveCurrentPredator (Actor|GetComponentbyClass _currentprey "/Game/Blueprints/AddOn/Components/BPC_Prey.BPC_Prey_C") (Components|GetOwner)))
        (:Is%20Not%20Valid
          _)))
    (:else
      _))
  (CallFunction|SetNearestPrey)
  (bind _currentprey_2 (Variables|Default|GetCurrentPrey)
    (:then
      (Utilities|IsValid (Actor|GetComponentbyClass _currentprey_2 "/Game/Blueprints/AddOn/Components/BPC_Prey.BPC_Prey_C")
        (:Is%20Valid
          (Default|AddCurrentPredator (Actor|GetComponentbyClass _currentprey_2 "/Game/Blueprints/AddOn/Components/BPC_Prey.BPC_Prey_C") (Components|GetOwner))
          (Default|CallEDHavetoHunt))))
    (:else)))

(event Custom|ED_OnComponentActive_Event
  (params (Active :type Boolean))
  (Components|Tick|SetComponentTickEnabled Active)
  (Variables|/Script/Engine.PrimitiveComponent|SetbGenerateOverlapEvents (Variables|Default|GetPredatorDetection) Active))

(event Custom|AddPreyInRange_Event
  (params (TargetInRange :type Actor%20Object%20Reference))
  (bind _actorsinarea (Variables|Default|GetActorsInArea))
  ;[0 1 0.1339] Ajoute Proie Quand Dans Collider
  (if (not (Utilities|Array|ContainsItem _actorsinarea TargetInRange))
    (Utilities|Array|Add _actorsinarea TargetInRange)
    (Game|BindEventtoOnDestroyed TargetInRange (EventDispatchers|CreateEvent :!event Custom|RemovePreyInRange_Event))
    (Game|BindEventtoOnDestroyed TargetInRange (EventDispatchers|CreateEvent :!event Custom|Event_RemovePreyToHunt_Event))))

(event Custom|RemovePreyInRange_Event
  (params (TargetOutRange :type Actor%20Object%20Reference))
  ;[0 1 0.1339] Ajoute Proie Quand Dans Collider
  (if (Utilities|Array|ContainsItem (Variables|Default|GetActorsInArea) TargetOutRange)
    (Utilities|Array|RemoveItem (Variables|Default|GetActorsInArea) TargetOutRange)
    (Game|UnbindEventfromOnDestroyed TargetOutRange (EventDispatchers|CreateEvent :!event Custom|RemovePreyInRange_Event))
    (Game|UnbindEventfromOnDestroyed TargetOutRange (EventDispatchers|CreateEvent :!event Custom|Event_RemovePreyToHunt_Event))))

(event Custom|Event_AddPreyToHunt_Event
  (params (PreyToHunt :type Actor%20Object%20Reference))
  (bind _actorsinsight (Variables|Default|GetActorsInSight))
  ;[1 0.2033 0] Chasse les proies visible
  (if (not (Utilities|Array|ContainsItem _actorsinsight PreyToHunt))
    (Utilities|Array|Add _actorsinsight PreyToHunt)
    (CallFunction|ChangePrey)
    (Default|CallEDAddPreytoHunt PreyToHunt)))

(event EventTick
  (params (DeltaSeconds :type Float%20%28single-precision%29))
  (if (CallFunction|HasPreyinRange)
    (for _array_element (Variables|Default|GetActorsInArea)
      (Utilities|IsValid _array_element
        (:Is%20Valid
          (if (CallFunction|TargetTooFar _array_element)
            (CallFunction|EventRemovePreytoHuntEvent _array_element)
            (else
              (CallFunction|EventAddPreytoHuntEvent _array_element)))
          (if (CallFunction|HasPreyinSight)
            (Default|CallEDHavetoHunt)))))))

(event EventBeginPlay
  (EventDispatchers|BindEventtoEDonComponentActive (EventDispatchers|CreateEvent :!event Custom|ED_OnComponentActive_Event)))

(event EventEndPlay
  (params (EndPlayReason :type EEndPlayReason%20Enum :default "Destroyed"))
  (bind _predatordetection (Variables|Default|GetPredatorDetection))
  ;[0 1 0.4676] Unbind Events
  (Utilities|IsValid _predatordetection
    (:Is%20Valid
      (EventDispatchers|UnbindallEventsfromOnComponentBeginOverlap _predatordetection)
      (EventDispatchers|UnbindallEventsfromOnComponentEndOverlap _predatordetection)
      (EventDispatchers|UnbindallEventsfromEDHavetoHunt))))

(fn Initialize
  (params (PredatorDetection :type Sphere%20Component%20Object%20Reference) (RangeEndDetection :type Float%20%28double-precision%29) (SizeSelf :type E_SizeType%20Enum :default "NewEnumerator3"))
  (Variables|Default|SetPredatorDetection PredatorDetection)
  (Variables|Default|SetSizeSelf SizeSelf)
  (Variables|Default|SetRange%20End%20Detection RangeEndDetection)
  (Utilities|IsValid (Variables|Default|GetPredatorDetection)
    (:Is%20Valid
      (Collision|BindEventtoOnComponentBeginOverlap (Variables|Default|GetPredatorDetection) (EventDispatchers|CreateEvent :!event Custom|OnBeginOverlap)))))

(fn IsAPrey
  (params (SizeType :type Byte))
  (return (< SizeType (Math|Byte|MakeLiteralByte (Variables|Default|GetSizeSelf)))))

(fn HasPreyinRange
  (return (Utilities|Array|IsNotEmpty (Variables|Default|GetActorsInArea))))

(fn SetNearestPrey
  (bind _actorsinsight (Variables|Default|GetActorsInSight))
  (Utilities|CurrentPreyExist
    (:CurrentPreyIsValid
      _)
    (:CurrentPreyIsNULL
      (for (_array_element _array_index) _actorsinsight
        (if (!= (LocalVariables|GetLowestDistance) -1.0)
          (if (< (Transformation|GetDistanceTo (Components|GetOwner) _array_element) (LocalVariables|GetLowestDistance))
            (LocalVariables|SetLowestDistance (Transformation|GetDistanceTo (Components|GetOwner) _array_element) :!label _label)
            (LocalVariables|SetIndexNearest _array_index))
          (else
            (goto _label))))
      (Variables|Default|SetCurrentPrey (Utilities|Array|Get(acopy) _actorsinsight (LocalVariables|GetIndexNearest)))))
  (return))

(fn IsVisible
  (params (Target :type Actor%20Object%20Reference%20%28by%20ref%29))
  (bind _outhit (Collision|LineTraceByChannel (Transformation|GetActorLocation (Components|GetOwner)) (Transformation|GetActorLocation Target) "TraceTypeQuery1" false (Variables|Default|GetActorsToIgnore) "None"))
  (return (== Target (.HitActor (Collision|BreakHitResult _outhit)))))

(fn GetPreyDirection
  (bind _currentprey (Variables|Default|GetCurrentPrey)
    (:then
      (return (Math|Vector|GetUnitDirection(Vector) (Transformation|GetActorLocation (Components|GetOwner)) (Transformation|GetActorLocation _currentprey))))
    (:else
      (Development|PrintText (Utilities|Text|FormatText "Prey not found") true true "(R=1.000000,G=0.085036,B=0.000000,A=1.000000)" 5.0)
      (return "0, 0, 0"))))

(fn HasPreyinSight
  (return (Utilities|Array|IsNotEmpty (Variables|Default|GetActorsInSight))))

(fn TargetTooFar
  (params (TargetActor :type Actor%20Object%20Reference))
  (return (> (Math|Vector|Distance(Vector) (Transformation|GetActorLocation TargetActor) (Transformation|GetActorLocation (Components|GetOwner))) (Variables|Default|GetRange%20End%20Detection))))

(fn HasPreyNear
  (params (Distance :type Float%20%28double-precision%29))
  (for _array_element (Variables|Default|GetActorsInSight)
    (if (<= (Math|Vector|Distance(Vector) (Transformation|GetActorLocation _array_element) (Transformation|GetActorLocation (Components|GetOwner))) Distance)
      (LocalVariables|SetPreyNear (<= (Math|Vector|Distance(Vector) (Transformation|GetActorLocation _array_element) (Transformation|GetActorLocation (Components|GetOwner))) Distance))
      (return (LocalVariables|GetPreyNear))))
  (return (LocalVariables|GetPreyNear)))

(fn AddActorstoSeeThrough
  (params (ActorToSeeThrough :type Actor%20Object%20Reference%20%28by%20ref%29))
  (bind _actorstoignore (Variables|Default|GetActorsToIgnore))
  (if (Utilities|Array|ContainsItem _actorstoignore ActorToSeeThrough)
    _
    (else
      (Utilities|Array|Add _actorstoignore ActorToSeeThrough)))
  (return))

(fn RemoveActorstoSeeThrough
  (params (ActorToSeeThrough :type Actor%20Object%20Reference%20%28by%20ref%29))
  (bind _actorstoignore (Variables|Default|GetActorsToIgnore))
  (if (Utilities|Array|ContainsItem _actorstoignore ActorToSeeThrough)
    (Utilities|Array|RemoveItem _actorstoignore ActorToSeeThrough))
  (return))