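; Actor component that gives its owner a shield rendered with the M_WaterShield material.
; Init adds a static mesh with a dynamic material, uses it or an added sphere component as the collider, and starts with zero alpha and no collision.
; Activation and deactivation functions switch collision profile and visibility, with deactivation also zeroing alpha.
; A separate function interpolates the material's alpha toward a target using frame delta time.
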(event Custom|Init
  (params (SphereSize :type Float%20%28double-precision%29) (Static%20Mesh :type Static%20Mesh%20Object%20Reference) (MeshScale :type Float%20%28single-precision%29))
  (bind _returnvalue (Rendering|Material|CreateDynamicMaterialInstance "/Game/VFX/Materials/Fish/M_WaterShield.M_WaterShield" "None" "None" :!class /Script/Engine.KismetMaterialLibrary))
  (bind _output_get (Variables|Default|SetMID_Shield _returnvalue))
  (CallFunction|CreateStaticMesh Static%20Mesh _output_get MeshScale)
  (Variables|Default|SetShieldCollision (Variables|Components|Created|GetMeshShieldRenderer))
  (if (Variables|Default|GetMeshIsCollider)
    _
    (else
      (CallFunction|CreateSphere SphereSize false)
      (Variables|Default|SetShieldCollision (Variables|Components|Created|GetShieldSphereCollision))))
  (Rendering|Material|SetScalarParameterValue (Variables|Default|GetMID_Shield) "Alpha" 0.0 :!class /Script/Engine.MaterialInstanceDynamic)
  (Collision|SetCollisionProfileName (Variables|Default|GetShieldCollision) "NoCollision" true :!class /Script/Engine.PrimitiveComponent))

(fn CreateSphere
  (params (InSphereRadius :type Float%20%28single-precision%29) (NewHidden :type Boolean))
  (bind _returnvalue (Game|AddComponentbyClass (Components|GetOwner) "/Script/Engine.SphereComponent" false))
  (bind _output_get (Variables|Components|Created|SetShieldSphereCollision _returnvalue))
  (Components|Sphere|SetSphereRadius _output_get InSphereRadius true)
  (Development|SetHiddeninGame _output_get NewHidden false)
  (Rendering|SetVisibility _output_get true false)
  (Class|ShapeComponent|SetLineThickness _output_get 5e+01)
  (return))

(fn CreateStaticMesh
  (params (Static%20Mesh :type Static%20Mesh%20Object%20Reference) (Material :type Material%20Instance%20Object%20Reference) (Scale :type Float%20%28single-precision%29))
  (bind _returnvalue (Game|AddComponentbyClass (Components|GetOwner) "/Script/Engine.StaticMeshComponent" false (Math|Transform|MakeTransform "0, 0, 0" "0, 0, 0" (* Scale "1.000000,1.000000,1.000000"))))
  (bind _output_get (Variables|Components|Created|SetMeshShieldRenderer _returnvalue))
  (Components|StaticMesh|SetStaticMesh _output_get Static%20Mesh)
  (Rendering|Material|SetMaterial _output_get 0 Material)
  (return))

(fn ActiveShield
  (params (IsActive :type Boolean))
  (if IsActive
    (LocalVariables|SetCurrentCollisionProfileName (Variables|ShieldState|GetShieldCollisionProfileName)))
  (Collision|SetCollisionProfileName (Variables|Default|GetShieldCollision) (LocalVariables|GetCurrentCollisionProfileName) true :!class /Script/Engine.PrimitiveComponent)
  (Development|SetHiddeninGame (Variables|Default|GetShieldCollision) (and (not (Variables|ShieldState|GetIs%20Active)) (Variables|ShieldState|GetIsHidden)) true) ; Affiche/ Desaffiche le shield
)

(fn SetActiveShield
  (params (IsActive :type Boolean))
  (LocalVariables|SetPreviousValue (Variables|ShieldState|GetIs%20Active))
  (Variables|ShieldState|SetIs%20Active IsActive)
  (if (!= (Variables|ShieldState|GetIs%20Active) (LocalVariables|GetPreviousValue))
    (if (Variables|ShieldState|GetIs%20Active)
      (CallFunction|ActiveShield (Variables|ShieldState|GetIs%20Active)))))

(fn SetMaterialOpacity
  (params (Target :type Float%20%28double-precision%29))
  (bind _mid_shield (Variables|Default|GetMID_Shield))
  (bind _returnvalue (Rendering|Material|GetScalarParameterValue _mid_shield "Alpha" :!class /Script/Engine.MaterialInstanceDynamic))
  (Rendering|Material|SetScalarParameterValue _mid_shield "Alpha" (Math|Interpolation|FInterpTo _returnvalue Target (Utilities|Time|GetWorldDeltaSeconds) (Variables|Default|GetInterpMaterialOpacity)) :!class /Script/Engine.MaterialInstanceDynamic))

(fn DeactiveShield
  (Collision|SetCollisionProfileName (Variables|Default|GetShieldCollision) "NoCollision" true :!class /Script/Engine.PrimitiveComponent)
  (Development|SetHiddeninGame (Variables|Default|GetShieldCollision) true true) ; Desaffiche le shield
  (Rendering|Material|SetScalarParameterValue (Variables|Default|GetMID_Shield) "Alpha" 0.0 :!class /Script/Engine.MaterialInstanceDynamic))