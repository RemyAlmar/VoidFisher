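; Component that manages a set of tools stored in an enum-keyed map and tracks which one is active.
; Toggle, switch, open and close functions change the active tool according to its lock, switchable and togglable flags.
; Use, hold, unlock and upgrade calls are forwarded to the tool objects' events, with manager-level dispatchers broadcasting these actions.
; It also offers level queries and bulk unlock or upgrade of every tool.
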(fn UnlockTool
  (params (ToolToUnlock :type E_ToolShip%20Enum :default "NewEnumerator3"))
  (bind _toollist (Variables|Default|GetToolList))
  (bind _value (Utilities|Map|Find _toollist ToolToUnlock))
  (Utilities|IsValid _value
    (:Is%20Valid
      (Default|EDUnlockToolEvent _value)
      (Default|CallEDonUnlockToolManager ToolToUnlock))
    (:Is%20Not%20Valid
      (Development|PrintText (Utilities|Text|FormatText "{name} don't exist in tool manager" (Utilities|String|EnumtoString ToolToUnlock))))))

(fn IsLock
  (params (Tool :type E_ToolShip%20Enum :default "NewEnumerator3"))
  (bind _toollist (Variables|Default|GetToolList))
  (bind (_value _returnvalue) (Utilities|Map|Find _toollist Tool))
  (if _returnvalue
    (LocalVariables|SetLIsLock (Variables|/Game/Blueprints/Game/Player/ToolsComponent/BPC_ToolBase.BPC_ToolBase_C|GetIsLock _value))
    (return (LocalVariables|GetLIsLock))))

(fn UseTool
  (bind _toollist (Variables|Default|GetToolList))
  (bind _currenttoolactive (Variables|Default|GetCurrentToolActive))
  (bind (_value _returnvalue) (Utilities|Map|Find _toollist _currenttoolactive))
  (if _returnvalue
    (if (Variables|/Game/Blueprints/Game/Player/ToolsComponent/BPC_ToolBase.BPC_ToolBase_C|GetCanUseTool _value)
      (Default|EDUseToolEvent _value)
      (Default|CallEDonUseToolManager (Variables|Default|GetCurrentToolActive)))))

(fn UseMaintainTool
  (params (TriggeredSeconds :type Float%20%28double-precision%29))
  (bind _toollist (Variables|Default|GetToolList))
  (bind _currenttoolactive (Variables|Default|GetCurrentToolActive))
  (bind (_value _returnvalue) (Utilities|Map|Find _toollist _currenttoolactive))
  (if _returnvalue
    (if (Variables|/Game/Blueprints/Game/Player/ToolsComponent/BPC_ToolBase.BPC_ToolBase_C|GetCanUseTool _value)
      (Default|EDHoldToolEvent _value TriggeredSeconds)
      (Default|CallEDonMaintainToolManager (Variables|Default|GetCurrentToolActive) TriggeredSeconds))))

(fn AddTool
  (params (Key :type E_ToolShip%20Enum%20%28by%20ref%29 :default "NewEnumerator3") (Value :type BPC%20Tool%20Base%20Object%20Reference%20%28by%20ref%29))
  (Utilities|Map|Add (Variables|Default|GetToolList) Key Value))

(fn OpenTool
  (params (ToolToOpen :type E_ToolShip%20Enum :default "NewEnumerator0"))
  (bind _toollist (Variables|Default|GetToolList))
  (bind (_value _returnvalue) (Utilities|Map|Find _toollist ToolToOpen))
  (if _returnvalue
    (Default|EDActiveToolEvent _value)
    (bind _output_get (Variables|Default|SetCurrentToolActive ToolToOpen))
    (Default|CallEDonActiveToolManager _output_get)
    (else
      (Development|PrintText (Utilities|Text|FormatText "WARNING : Tool Missing {name}" (Utilities|String|EnumtoString ToolToOpen)) true true "(R=1.000000,G=0.587717,B=0.000000,A=1.000000)" 5.0))))

(fn CloseTool
  (params (ToolToClosed :type E_ToolShip%20Enum :default "NewEnumerator0") (ToolToActive :type E_ToolShip%20Enum :default "NewEnumerator3"))
  (bind _toollist (Variables|Default|GetToolList))
  (bind (_value _returnvalue) (Utilities|Map|Find _toollist ToolToClosed))
  (if _returnvalue
    (if (ToolManaging|AlreadyActive ToolToActive)
      (if (Variables|/Game/Blueprints/Game/Player/ToolsComponent/BPC_ToolBase.BPC_ToolBase_C|GetIsTogglable _value)
        (Default|EDDeactiveToolEvent _value :!label _label)
        (Default|CallEDonDeactiveToolManager ToolToClosed)
        (Variables|Default|SetCurrentToolActive "NewEnumerator3")
        (else
          (Default|EDActiveToolEvent _value)
          (Default|CallEDonActiveToolManager ToolToActive)))
      (else
        (goto _label)))))

(fn SwitchTool
  (params (NewTool :type E_ToolShip%20Enum :default "NewEnumerator0"))
  (bind _toollist (Variables|Default|GetToolList))
  (bind _value (Utilities|Map|Find _toollist NewTool))
  (if (Variables|/Game/Blueprints/Game/Player/ToolsComponent/BPC_ToolBase.BPC_ToolBase_C|GetSwitchable _value)
    (ToolManaging|CloseTool (Variables|Default|GetCurrentToolActive) NewTool)
    (ToolManaging|OpenTool NewTool)
    (else
      (Default|EDActiveToolEvent _value))))

(fn AlreadyActive
  (params (ToolToActive :type E_ToolShip%20Enum :default "NewEnumerator3"))
  (return (Utilities|Enum|Equal(Enum) ToolToActive (Variables|Default|GetCurrentToolActive))))

(fn ToggleTool
  (params (NextTool :type E_ToolShip%20Enum :default "NewEnumerator3"))
  (if (ToolLock|IsLock NextTool)
    (ToolManaging|CloseTool (Variables|Default|GetCurrentToolActive) NextTool :!label _label)
    (elif (ToolManaging|AlreadyActive NextTool)
      (goto _label)
      (else
        (ToolManaging|SwitchTool NextTool)))))

(fn GetCurrentLevel
  (params (Tool :type E_ToolShip%20Enum :default "NewEnumerator3"))
  (bind _toollist (Variables|Default|GetToolList))
  (bind (_value _returnvalue) (Utilities|Map|Find _toollist Tool))
  (if _returnvalue
    (LocalVariables|SetLCurrentLevel (Variables|/Game/Blueprints/Game/Player/ToolsComponent/BPC_ToolBase.BPC_ToolBase_C|GetCurrentLevel _value))
    (return (LocalVariables|GetLCurrentLevel))))

(fn GetNextLevel
  (params (Tool :type E_ToolShip%20Enum :default "NewEnumerator3") (NextValue :type Integer))
  (bind _toollist (Variables|Default|GetToolList))
  (bind (_value _returnvalue) (Utilities|Map|Find _toollist Tool))
  (if _returnvalue
    (return (Variables|/Game/Blueprints/Game/Player/ToolsComponent/BPC_ToolBase.BPC_ToolBase_C|GetCurrentLevel _value))))

(fn UpgradeTool
  (params (ToolToUpgrade :type E_ToolShip%20Enum :default "NewEnumerator3"))
  (Default|EDUpgradeNextLevelEvent (.Value (Utilities|Map|Find (Variables|Default|GetToolList) ToolToUpgrade)))
  (Default|CallEDonUpgradeToolManager ToolToUpgrade))

(fn GetTotalLevel
  (params (Tool :type E_ToolShip%20Enum :default "NewEnumerator3"))
  (bind _toollist (Variables|Default|GetToolList))
  (bind (_value _returnvalue) (Utilities|Map|Find _toollist Tool))
  (if _returnvalue
    (LocalVariables|SetCurrentLevel (Default|GetTotalLevel _value))
    (return (LocalVariables|GetCurrentLevel))))

(fn CanUpgradeTool
  (params (ToolTarget :type E_ToolShip%20Enum :default "NewEnumerator3"))
  (bind _output_get (LocalVariables|SetCurrentTool (.Value (Utilities|Map|Find (Variables|Default|GetToolList) ToolTarget))))
  (Utilities|IsValid _output_get
    (:Is%20Valid
      (if (not (Variables|/Game/Blueprints/Game/Player/ToolsComponent/BPC_ToolBase.BPC_ToolBase_C|GetIsLock (LocalVariables|GetCurrentTool)))
        (LocalVariables|SetCanUpgrade (Default|CanbeUpgrade (LocalVariables|GetCurrentTool)))
        (return (LocalVariables|GetCanUpgrade))))))

(fn StopMaintainTool
  (params (TriggeredSeconds :type Float%20%28double-precision%29))
  (bind _toollist (Variables|Default|GetToolList))
  (bind _currenttoolactive (Variables|Default|GetCurrentToolActive))
  (bind (_value _returnvalue) (Utilities|Map|Find _toollist _currenttoolactive))
  (if _returnvalue
    (Default|EDStopHoldToolEvent _value TriggeredSeconds)
    (Default|CallEDonStopMaintainToolManager (Variables|Default|GetCurrentToolActive) TriggeredSeconds)))

(fn UpgradeAllTools
  (bind _keys (Utilities|Map|Keys (Variables|Default|GetToolList)))
  (for _array_element _keys
    (ToolLevel|UpgradeTool _array_element)))

(fn UnlockAllTools
  (bind _keys (Utilities|Map|Keys (Variables|Default|GetToolList)))
  (for _array_element _keys
    (ToolLock|UnlockTool _array_element)))

(fn CloseCurrentTool
  (Default|EDDeactiveToolEvent (ToolManaging|GetCurrentTool))
  (Default|CallEDonDeactiveToolManager (Variables|Default|GetCurrentToolActive))
  (Variables|Default|SetCurrentToolActive "NewEnumerator3"))

(fn GetCurrentTool
  (bind _output_get (LocalVariables|SetCurrentTool (.Value (Utilities|Map|Find (Variables|Default|GetToolList) (Variables|Default|GetCurrentToolActive)))))
  (Utilities|IsValid _output_get
    (:Is%20Valid
      _)
    (:Is%20Not%20Valid
      (LocalVariables|SetCurrentTool (.Value (Utilities|Map|Find (Variables|Default|GetToolList) "NewEnumerator2")))))
  (return (LocalVariables|GetCurrentTool)))