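; Health manager component that currently handles collision response and an invulnerability timer, with no health value in its graph.
; BeginPlay finds the owner's BPC_ActorPhysicsMovement and binds to its root hit event.
; Each hit adjusts speed from the impact normal and, while invulnerable, adds a speed-scaled, reflection-style bounce impulse.
; Tick prints and advances the timer that clears invulnerability, but the only code setting it is disconnected.
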(event Custom|Root_OnComponentHit
  (params (HitComponent :type Primitive%20Component%20Object%20Reference) (OtherActor :type Actor%20Object%20Reference) (OtherComp :type Primitive%20Component%20Object%20Reference) (NormalImpulse :type Vector) (Hit :type Hit%20Result%20Structure%20%28by%20ref%29))
  (bind _impactnormal (Collision|BreakHitResult Hit))
  (bind _bpc_actorphysics (Variables|Default|GetBPC_ActorPhysics))
  (bind _bpc_actorphysics_2 (Variables|Default|GetBPC_ActorPhysics))
  (bind _ownrootphysics (Variables|/Game/Blueprints/AddOn/Components/BPC_ActorPhysicsMovement.BPC_ActorPhysicsMovement_C|GetOwnRootPhysics _bpc_actorphysics_2))
  (Default|ChangeSpeedonImpact _bpc_actorphysics _impactnormal)
  (if (Variables|Invulnerability|GetIsInvulnerable)
    (Physics|AddImpulse _ownrootphysics (* (- (CallFunction|GetVelocity _ownrootphysics) (* (* (Math|Vector|DotProduct (Math|Vector|GetForwardVector (Variables|/Game/Blueprints/AddOn/Components/BPC_ActorPhysicsMovement.BPC_ActorPhysicsMovement_C|GetOwnRootPhysics _bpc_actorphysics)) _impactnormal) _impactnormal) 2.0)) (Variables|/Game/Blueprints/AddOn/Components/BPC_ActorPhysicsMovement.BPC_ActorPhysicsMovement_C|GetCurrentSpeed _bpc_actorphysics)) "None" false)))

(event EventTick
  (params (DeltaSeconds :type Float%20%28single-precision%29))
  (Development|PrintText (Utilities|Text|FormatText "{x} / {y} s Invulnerable" (Variables|Invulnerability|Time|GetCurrentTime_Invulnerability) (Variables|Invulnerability|Time|GetMaxTime_Invulnerability)) true true "(R=1.000000,G=0.000000,B=0.354175,A=1.000000)" 0.0)
  (if (Variables|Invulnerability|GetIsInvulnerable)
    (if (CallFunction|TimerPos (Variables|Invulnerability|Time|GetCurrentTime_Invulnerability) (Variables|Invulnerability|Time|GetMaxTime_Invulnerability) 1.0 true)
      (Variables|Invulnerability|SetIsInvulnerable false))))

(event EventBeginPlay
  (bind _returnvalue (Components|GetOwner))
  (bind _returnvalue_2 (Actor|GetComponentbyClass _returnvalue "/Game/Blueprints/AddOn/Components/BPC_ActorPhysicsMovement.BPC_ActorPhysicsMovement_C"))
  (Utilities|IsValid _returnvalue_2
    (:Is%20Valid
      (bind _output_get (Variables|Default|SetBPC_ActorPhysics _returnvalue_2))
      (Collision|BindEventtoOnComponentHit (Variables|/Game/Blueprints/AddOn/Components/BPC_ActorPhysicsMovement.BPC_ActorPhysicsMovement_C|GetOwnRootPhysics _output_get) (EventDispatchers|CreateEvent :!event Custom|Root_OnComponentHit)))))