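; Actor component that serves creature data and holds per-type catch counts, weights and sizes.
; On BeginPlay it seeds the three maps with zeros for every DT_CreatureDetails row, keyed by creature enum.
; Lookups index table rows by enum value, so row order must match the enum.
; Helpers add catches, sum maps and compute averages; the "Median" functions are means, with per-creature values divided by catch count.
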(event EventBeginPlay
  ;[0 0 0] instance DATA
  (CallFunction|Initialization))

(fn GetAllData
  (params (CreatureType :type E_CreatureType%20Enum :default "NewEnumerator3"))
  (bind _outrownames (DataTable|GetDataTableRowNames "/Game/Blueprints/Data/DataTable/DT_CreatureDetails.DT_CreatureDetails"))
  (bind _returnvalue (Utilities|GetDataTableRow "/Game/Blueprints/Data/DataTable/DT_CreatureDetails.DT_CreatureDetails" (Utilities|Array|Get(acopy) _outrownames (Math|Conversions|ToInteger(Byte) CreatureType)))
    (:then
      (return _returnvalue))))

(fn GetDescription
  (params (CreatureType :type E_CreatureType%20Enum :default "NewEnumerator3"))
  (return (.creaturedescription (Get|GetAllData CreatureType))))

(fn GetTotalValue
  (params (TargetMap :type Map%20of%20E_CreatureType%20Enums%20to%20Integers :default "NewEnumerator4"))
  (LocalVariables|SetTotal 0)
  (bind _values (Utilities|Map|Values TargetMap))
  (for _array_element _values
    (LocalVariables|SetTotal (+ _array_element (LocalVariables|GetTotal))))
  (return (LocalVariables|GetTotal)))

(fn GetCreatureNumberCatched
  (params (Key :type E_CreatureType%20Enum%20%28by%20ref%29 :default "NewEnumerator4"))
  (bind _creaturetypecatched (Variables|Statistics|GetCreatureTypeCatched))
  (bind (_value _returnvalue) (Utilities|Map|Find _creaturetypecatched Key))
  (if _returnvalue
    (return _value)))

(fn AddCreatureCatched
  (params (TargetToAdd :type E_CreatureType%20Enum%20%28by%20ref%29 :default "NewEnumerator4") (QuantityToAdd :type Integer))
  (bind _creaturetypecatched (Variables|Statistics|GetCreatureTypeCatched))
  (Utilities|Map|Add _creaturetypecatched TargetToAdd (+ QuantityToAdd (.Value (Utilities|Map|Find _creaturetypecatched TargetToAdd)))))

(fn Initialization
  (bind _outrownames (DataTable|GetDataTableRowNames "/Game/Blueprints/Data/DataTable/DT_CreatureDetails.DT_CreatureDetails"))
  (for _array_element _outrownames
    (bind _returnvalue (Utilities|GetDataTableRow "/Game/Blueprints/Data/DataTable/DT_CreatureDetails.DT_CreatureDetails" _array_element)
      (:then
        (Utilities|Map|Add (Variables|Statistics|GetCurrentCreatureWeight) (Utilities|Enum|ByteToEnumE_CreatureType (.creaturename _returnvalue)) 0.0)
        (Utilities|Map|Add (Variables|Statistics|GetCreatureTypeCatched) (Utilities|Enum|ByteToEnumE_CreatureType (.creaturename _returnvalue)) 0)
        (Utilities|Map|Add (Variables|Statistics|GetCurrentCreatureSize) (Utilities|Enum|ByteToEnumE_CreatureType (.creaturename _returnvalue)) 0.0)))))

(fn GetMedianTotalArray
  (params (TargetMap :type Map%20of%20E_CreatureType%20Enums%20to%20Reals :default "NewEnumerator4"))
  (LocalVariables|SetMedianValue 0.0)
  (bind _values (Utilities|Map|Values TargetMap))
  (for _array_element _values
    (LocalVariables|SetMedianValue (+ _array_element (LocalVariables|GetMedianValue))))
  (return (Math|Float|SafeDivide (LocalVariables|GetMedianValue) (Math|Conversions|ToFloat(Integer) (Utilities|Map|Length TargetMap)))))

(fn GetMedian
  (params (Value :type Float%20%28double-precision%29) (Divider :type Float%20%28double-precision%29))
  (return (Math|Float|SafeDivide Value Divider)))

(fn GetMedianCreature
  (params (TargetMap :type Map%20of%20E_CreatureType%20Enums%20to%20Reals :default "NewEnumerator4") (Target :type E_CreatureType%20Enum%20%28by%20ref%29 :default "NewEnumerator4"))
  (bind (_value _returnvalue) (Utilities|Map|Find TargetMap Target))
  (bind _creaturetypecatched (Variables|Statistics|GetCreatureTypeCatched))
  (bind (_value_2 _returnvalue_2) (Utilities|Map|Find _creaturetypecatched Target))
  (if (and _returnvalue _returnvalue_2)
    (return (Get|GetMedian _value (Math|Conversions|ToFloat(Integer) _value_2)))))