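; Prey component that lets a creature detect and track larger predators and supplies an averaged direction to flee from them.
; Overlaps on the detection primitive passed to Initialize register visible BPC_Predator actors of greater size.
; While active, Tick drops distant threats, updates which are seen via line traces with an ignore list, and fires seen, in/out, afraid and no-predator dispatchers.
; It also keeps a list of predators currently aiming at it.
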(event Custom|ED_ReactOnPredatorOut_Event
  (params (TargetPredator :type Actor%20Object%20Reference))
  ;[1 0.1713 0.3724] Divers Event Dispatcher
)

(event Custom|OnBeginOverlapPredatorDetection
  (params (OverlappedComponent :type Primitive%20Component%20Object%20Reference) (OtherActor :type Actor%20Object%20Reference) (OtherComp :type Primitive%20Component%20Object%20Reference) (OtherBodyIndex :type Integer) (bFromSweep :type Boolean) (SweepResult :type Hit%20Result%20Structure%20%28by%20ref%29))
  (bind _returnvalue (Actor|GetComponentbyClass OtherActor "/Game/Blueprints/AddOn/Components/BPC_Predator.BPC_Predator_C"))
  (bind _actorstoflee (Variables|Default|GetActorsToFlee))
  ;[0 0.4408 1] Entrée et Sortie des predator à portée de la créature
  (Utilities|IsValid _returnvalue
    (:Is%20Valid
      (if (CallFunction|ThisAPredator (Variables|/Game/Blueprints/AddOn/Components/BPC_Predator.BPC_Predator_C|GetSizeSelf _returnvalue))
        (if (CallFunction|IsVisible OtherActor)
          (if (not (Utilities|Array|ContainsItem _actorstoflee OtherActor))
            (Utilities|Array|Add _actorstoflee OtherActor)))))))

(event Custom|ED_SeePredatorInRange_Event
  (params (TargetPredator :type Actor%20Object%20Reference))
  ;[1 0.1713 0.3724] Divers Event Dispatcher
)

(event Custom|ED_IsAimed_Event
  ;[1 0.1713 0.3724] Divers Event Dispatcher
)

(event Custom|ED_ReactOnPredatorIn_Event
  (params (TargetPredator :type Actor%20Object%20Reference))
  ;[1 0.1713 0.3724] Divers Event Dispatcher
)

(event Custom|ED_OnComponentActive_Event
  (params (Active :type Boolean))
  (bind _predatordetection (Variables|Default|GetPredatorDetection))
  (Variables|/Script/Engine.PrimitiveComponent|SetbGenerateOverlapEvents _predatordetection Active)
  (Components|Activation|SetActive _predatordetection Active false)
  (Components|Tick|SetComponentTickEnabled Active))

(event EventTick
  (params (DeltaSeconds :type Float%20%28single-precision%29))
  (if (CallFunction|HasPredatorinRange)
    (CallFunction|HandlePredatorinRange)
    (if (CallFunction|HasAPredatorSeeing)
      (Default|CallEDIsAfraid))))

(event EventEndPlay
  (params (EndPlayReason :type EEndPlayReason%20Enum :default "Destroyed"))
  (bind _predatordetection (Variables|Default|GetPredatorDetection))
  ;[1 0.5145 0] Delink des events quand Composant detruit
  (Utilities|IsValid _predatordetection
    (:Is%20Valid
      (EventDispatchers|UnbindallEventsfromOnComponentBeginOverlap _predatordetection)
      (EventDispatchers|UnbindallEventsfromOnComponentEndOverlap _predatordetection)
      (EventDispatchers|UnbindallEventsfromEDSeePredatorinRange))))

(event EventBeginPlay
  (EventDispatchers|BindEventtoEDSeePredatorinRange (EventDispatchers|CreateEvent :!event Custom|ED_SeePredatorInRange_Event))
  (EventDispatchers|BindEventtoEDIsAimed (EventDispatchers|CreateEvent :!event Custom|ED_IsAimed_Event))
  (EventDispatchers|BindEventtoEDReactonPredatorin (EventDispatchers|CreateEvent :!event Custom|ED_ReactOnPredatorIn_Event))
  (EventDispatchers|BindEventtoEDReactonPredatorOut (EventDispatchers|CreateEvent :!event Custom|ED_ReactOnPredatorOut_Event))
  (EventDispatchers|BindEventtoEDonComponentActive (EventDispatchers|CreateEvent :!event Custom|ED_OnComponentActive_Event)))

(fn ThisAPredator
  (params (SizeOther :type Byte))
  (return (> SizeOther (Math|Byte|MakeLiteralByte (Variables|Default|GetSizeSelf)))))

(fn Initialize
  (params (TargetPredatorDetection :type Sphere%20Component%20Object%20Reference) (SizeSelf :type E_SizeType%20Enum :default "NewEnumerator3") (StopDetection :type Float%20%28double-precision%29))
  (Variables|Default|SetPredatorDetection TargetPredatorDetection)
  (Variables|Default|SetSizeSelf SizeSelf)
  (Variables|Default|SetDistToStopDetection StopDetection)
  (Collision|BindEventtoOnComponentBeginOverlap (Variables|Default|GetPredatorDetection) (EventDispatchers|CreateEvent :!event Custom|OnBeginOverlapPredatorDetection)))

(fn DirectiontoFlee
  (for _array_element (Variables|Default|GetActorsToFlee)
    (LocalVariables|SetMedianDirection (+ (Math|Vector|GetUnitDirection(Vector) (Transformation|GetActorLocation _array_element) (Transformation|GetActorLocation (Components|GetOwner))) (LocalVariables|GetMedianDirection))))
  (return (Math|Vector|Normalize (/ (LocalVariables|GetMedianDirection) (Utilities|Array|Length (Variables|Default|GetActorsToFlee))))))

(fn HasPredatorinRange
  (return (Utilities|Array|IsNotEmpty (Variables|Default|GetActorsToFlee))))

(fn IsVisible
  (params (Target :type Actor%20Object%20Reference%20%28by%20ref%29))
  (bind _outhit (Collision|LineTraceByChannel (Transformation|GetActorLocation (Components|GetOwner)) (Transformation|GetActorLocation Target) "TraceTypeQuery1" false (Variables|Default|GetActorsToIgnore) "None" true "(R=1.000000,G=0.000000,B=0.910864,A=1.000000)" "(R=0.000000,G=1.000000,B=0.770152,A=1.000000)" 0.0))
  (return (== Target (.HitActor (Collision|BreakHitResult _outhit)))))

(fn IsAimed
  (return (Utilities|Array|IsNotEmpty (Variables|Default|GetCurrentPredator))))

(fn AddCurrentPredator
  (params (PredatorAdded :type Actor%20Object%20Reference%20%28by%20ref%29))
  (bind _currentpredator (Variables|Default|GetCurrentPredator))
  (if (not (Utilities|Array|ContainsItem _currentpredator PredatorAdded))
    (Utilities|Array|Add _currentpredator PredatorAdded)))

(fn RemoveCurrentPredator
  (params (PredatorRemoved :type Actor%20Object%20Reference%20%28by%20ref%29))
  (bind _currentpredator (Variables|Default|GetCurrentPredator))
  (if (Utilities|Array|ContainsItem _currentpredator PredatorRemoved)
    (Utilities|Array|RemoveItem _currentpredator PredatorRemoved)))

(fn HandlePredatorinRange
  (for _array_element (Variables|Default|GetActorsToFlee)
    (bind _output_get (LocalVariables|SetL_CurrentPredator _array_element))
    (if (CallFunction|TargetTooFar _output_get)
      (CallFunction|RemoveActortoFlee (LocalVariables|GetL_CurrentPredator))
      (CallFunction|RemovePredatorSeeing (LocalVariables|GetL_CurrentPredator))
      (elif (CallFunction|IsVisible (LocalVariables|GetL_CurrentPredator))
        (CallFunction|AddPredatorSeeing (LocalVariables|GetL_CurrentPredator))
        (Default|CallEDSeePredatorinRange (LocalVariables|GetL_CurrentPredator))
        (else
          (CallFunction|RemovePredatorSeeing (LocalVariables|GetL_CurrentPredator))))))
  (return))

(fn HasAPredatorSeeing
  (return (Utilities|Array|IsNotEmpty (Variables|Default|GetActorSeeing))))

(fn AddPredatorSeeing
  (params (Actor :type Actor%20Object%20Reference%20%28by%20ref%29))
  (LocalVariables|SetCurrentActor Actor)
  (if (Utilities|Array|ContainsItem (Variables|Default|GetActorSeeing) (LocalVariables|GetCurrentActor))
    _
    (else
      (Utilities|Array|Add (Variables|Default|GetActorSeeing) (LocalVariables|GetCurrentActor))
      (Default|CallEDReactonPredatorin (LocalVariables|GetCurrentActor))))
  (return))

(fn RemovePredatorSeeing
  (params (TargetActor :type Actor%20Object%20Reference%20%28by%20ref%29))
  (bind _actorseeing (Variables|Default|GetActorSeeing))
  (LocalVariables|SetLCurrentPredator TargetActor)
  (if (Utilities|Array|ContainsItem _actorseeing (LocalVariables|GetLCurrentPredator))
    (Utilities|Array|RemoveItem _actorseeing (LocalVariables|GetLCurrentPredator))
    (Default|CallEDReactonPredatorOut (LocalVariables|GetLCurrentPredator)))
  (if (CallFunction|HasPredatorinRange)
    _
    (else
      (Utilities|Array|Clear (Variables|Default|GetActorSeeing))))
  (return))

(fn TargetTooFar
  (params (TargetActor :type Actor%20Object%20Reference))
  (return (> (Math|Vector|Distance(Vector) (Transformation|GetActorLocation TargetActor) (Transformation|GetActorLocation (Components|GetOwner))) (Variables|Default|GetDistToStopDetection))))

(fn RemoveActortoFlee
  (params (TargetPredator :type Actor%20Object%20Reference))
  (Utilities|Array|RemoveItem (Variables|Default|GetActorsToFlee) TargetPredator)
  (if (Utilities|Array|IsEmpty (Variables|Default|GetActorsToFlee))
    (Default|CallEDIsWithoutPredator))
  (return))

(fn HasPredatorNear
  (params (Distance :type Float%20%28double-precision%29))
  (for _array_element (Variables|Default|GetActorSeeing)
    (if (<= (Math|Vector|Distance(Vector) (Transformation|GetActorLocation _array_element) (Transformation|GetActorLocation (Components|GetOwner))) Distance)
      (LocalVariables|SetPredatorNear (<= (Math|Vector|Distance(Vector) (Transformation|GetActorLocation _array_element) (Transformation|GetActorLocation (Components|GetOwner))) Distance))
      (return (LocalVariables|GetPredatorNear))))
  (return (LocalVariables|GetPredatorNear)))

(fn RemoveActorstoSeeThrough
  (params (ActorToSeeThrough :type Actor%20Object%20Reference%20%28by%20ref%29))
  (bind _actorstoignore (Variables|Default|GetActorsToIgnore))
  (if (Utilities|Array|ContainsItem _actorstoignore ActorToSeeThrough)
    (Utilities|Array|RemoveItem _actorstoignore ActorToSeeThrough))
  (return))

(fn AddActorstoSeeThrough
  (params (ActorToSeeThrough :type Actor%20Object%20Reference%20%28by%20ref%29))
  (bind _actorstoignore (Variables|Default|GetActorsToIgnore))
  (if (Utilities|Array|ContainsItem _actorstoignore ActorToSeeThrough)
    _
    (else
      (Utilities|Array|Add _actorstoignore ActorToSeeThrough)))
  (return))