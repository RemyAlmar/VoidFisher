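; Generic component that stores named numeric parameters in a map on its owning actor.
; Bulk adds either overwrite existing keys or only fill in missing ones, and SetParams replaces the whole map.
; Single-value writes only update existing keys, printing the owner, component and name when one is missing.
; Getters read values as raw numbers, rounded ints, non-zero bools, or 2D and 3D vectors built from separate keys.
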(fn AddParamswithModify
  (params (ListToAdd :type Map%20of%20Strings%20to%20Reals))
  (bind _keys (Utilities|Map|Keys ListToAdd))
  (for _array_element _keys
    (Utilities|Map|Add (Variables|Default|GetParams) _array_element (.Value (Utilities|Map|Find ListToAdd _array_element))))
  (return))

(fn AddParamsWithoutModify
  (params (ListToAdd :type Map%20of%20Strings%20to%20Reals))
  (bind _keys (Utilities|Map|Keys ListToAdd))
  (LocalVariables|SetKeysToAdd _keys)
  (bind _values (Utilities|Map|Values ListToAdd))
  (LocalVariables|SetValuesToAdd _values)
  (bind _keys_2 (Utilities|Map|Keys (Variables|Default|GetParams)))
  (LocalVariables|SetCurrentKeys _keys_2)
  (for (_array_element _array_index) (LocalVariables|GetKeysToAdd)
    (LocalVariables|SetCurrentIndex _array_index)
    (if (not (Utilities|Array|ContainsItem (LocalVariables|GetCurrentKeys) _array_element))
      (Utilities|Map|Add (Variables|Default|GetParams) (Utilities|Array|Get(acopy) (LocalVariables|GetKeysToAdd) (LocalVariables|GetCurrentIndex)) (Utilities|Array|Get(acopy) (LocalVariables|GetValuesToAdd) (LocalVariables|GetCurrentIndex))))))

(fn SetParams
  (params (Params :type Map%20of%20Strings%20to%20Reals))
  (Variables|Default|SetParams Params)
  (return))

(fn GetParambyName
  (params (ParamName :type String))
  (return (.Value (Utilities|Map|Find (Variables|Default|GetParams) ParamName))))

(fn SetParambyName
  (params (ParamName :type String) (Value :type Float%20%28double-precision%29))
  (bind _params (Variables|Default|GetParams))
  (if (.ReturnValue (Utilities|Map|Find _params ParamName))
    (Utilities|Map|Add _params ParamName Value)
    (else
      (Development|PrintText (Utilities|Text|FormatText "({x}->{y}) Don't find param name of {z}" (Utilities|GetDisplayName (Components|GetOwner)) (Utilities|GetDisplayName self) ParamName) true true "(R=1.000000,G=0.000000,B=0.018721,A=1.000000)" 5.0)))
  (return))

(fn GetVector3byParamsName
  (params (NameX :type String) (NameY :type String) (NameZ :type String))
  (bind _params (Variables|Default|GetParams))
  (return (Math|Vector|MakeVector (.Value (Utilities|Map|Find _params NameX)) (.Value (Utilities|Map|Find _params NameY)) (.Value (Utilities|Map|Find _params NameZ)))))

(fn GetVector2byParamsName
  (params (NameX :type String) (NameY :type String))
  (bind _params (Variables|Default|GetParams))
  (return (Math|Vector2D|MakeVector2D (.Value (Utilities|Map|Find _params NameX)) (.Value (Utilities|Map|Find _params NameY)))))

(fn GetIntbyParamsName
  (params (ParamName :type String%20%28by%20ref%29))
  (return (Math|Float|Round (.Value (Utilities|Map|Find (Variables|Default|GetParams) ParamName)))))

(fn GetBoolbyParamName
  (params (Key :type String))
  (return (!= (.Value (Utilities|Map|Find (Variables|Default|GetParams) Key)) 0.0)))