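; BPC_StateStarter is a debug component that starts and drives the state manager components on its owning actor.
; On BeginPlay it caches every BPC_StateManager on the owner, deactivates each, initializes it with ListStatesClass, then reactivates it without a reset.
; Each Tick it forwards DeltaSeconds to every cached manager through IUpdate, so this component supplies their update loop.
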(event EventBeginPlay
  (bind _output_get (Variables|Default|SetStateManager (Actor|GetComponentsByClass (Components|GetOwner) "/Game/Blueprints/AddOn/Components/BPC_StateManager.BPC_StateManager_C")))
  (for _array_element _output_get
    (Components|Activation|SetActive _array_element false false)
    (Default|Initialize _array_element (Variables|Default|GetList%20States%20Class))
    (Components|Activation|SetActive _array_element true false)))

(event EventTick
  (params (DeltaSeconds :type Float%20%28single-precision%29))
  (for _array_element (Variables|Default|GetStateManager)
    (Default|IUpdate _array_element DeltaSeconds)))