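; Generic actor component that tracks which BP_Spline in the level its owner is associated with.
; BeginPlay caches every BP_Spline; GetCurrentSpline returns the stored spline or, if invalid, picks and keeps the one nearest the owner.
; SetCurrentSpline overrides that choice.
; The component moves nothing itself: Tick only has an empty check, and the look-ahead and sampled-point debug drawing is disconnected.
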(event EventTick
  (params (DeltaSeconds :type Float%20%28single-precision%29))
  (if (Utilities|Array|IsNotEmpty (Variables|Default|GetSplines))
    _))

(event EventBeginPlay
  (bind _outactors (Actor|GetAllActorsOfClass "/Game/Blueprints/Game/Miscellanious/BP_Spline.BP_Spline_C"))
  (Variables|Default|SetSplines _outactors))

(fn GetNearestSpline
  (bind _splines (Variables|Default|GetSplines))
  (bind _output (Utilities|Array|Get(acopy) _splines))
  (if (Utilities|Array|IsNotEmpty (Variables|Default|GetSplines))
    (LocalVariables|SetPreviousDistance (Default|GetDistancetoSpline _output (Transformation|GetActorLocation (Components|GetOwner))))
    (LocalVariables|SetNearestSpline _output)
    (for _array_element (Variables|Default|GetSplines)
      (if (< (Default|GetDistancetoSpline _array_element (Transformation|GetActorLocation (Components|GetOwner))) (LocalVariables|GetPreviousDistance))
        (LocalVariables|SetNearestSpline _array_element)
        (LocalVariables|SetPreviousDistance (Default|GetDistancetoSpline _array_element (Transformation|GetActorLocation (Components|GetOwner))))))
    (return (LocalVariables|GetNearestSpline))))

(fn GetCurrentSpline
  (Variables|Default|GetCurrentSpline
    (:then
      _)
    (:else
      (Variables|Default|SetCurrentSpline (CallFunction|GetNearestSpline))))
  (return (Variables|Default|GetCurrentSpline)))

(fn SetCurrentSpline
  (params (CurrentSpline :type BP%20Spline%20Object%20Reference))
  (Variables|Default|SetCurrentSpline CurrentSpline)
  (return))