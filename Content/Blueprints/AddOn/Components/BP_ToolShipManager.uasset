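; Ship tool manager that keeps a map of tools by enum and tracks which single one is active.
; It forwards open, close, use, secondary use, unlock and upgrade calls to the matching tool through event dispatchers, then broadcasts its own manager-level dispatcher.
; Toggling closes the current tool if the requested one is locked or already active, otherwise switches to it.
; Tools initialize when added, and getters expose lock state and level.
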(fn OpenTool
  (params (ToolToOpen :type E_ToolShip%20Enum :default "NewEnumerator0"))
  (bind _toollist (Variables|Default|GetToolList))
  (bind (_value _returnvalue) (Utilities|Map|Find _toollist ToolToOpen))
  (if _returnvalue
    (Default|CallEDActiveTool _value)
    (bind _output_get (Variables|Default|SetCurrentToolActive ToolToOpen))
    (Default|CallEDonActiveToolManager _output_get)
    (else
      (Development|PrintText (Utilities|Text|FormatText "WARNING : Tool Missing {name}" (Utilities|String|EnumtoString ToolToOpen)) true true "(R=1.000000,G=0.587717,B=0.000000,A=1.000000)" 5.0))))

(fn CloseTool
  (params (ToolToClosed :type E_ToolShip%20Enum :default "NewEnumerator0"))
  (bind _toollist (Variables|Default|GetToolList))
  (bind (_value _returnvalue) (Utilities|Map|Find _toollist ToolToClosed))
  (if _returnvalue
    (Default|CallEDDeactiveTool _value)
    (Default|CallEDonDeactiveToolManager ToolToClosed)
    (Variables|Default|SetCurrentToolActive "NewEnumerator3")))

(fn UnlockTool
  (params (ToolToUnlock :type E_ToolShip%20Enum :default "NewEnumerator3"))
  (Default|CallEDUnlockTool (.Value (Utilities|Map|Find (Variables|Default|GetToolList) ToolToUnlock)))
  (Default|CallEDonUnlockToolManager ToolToUnlock))

(fn UseTool
  (bind _toollist (Variables|Default|GetToolList))
  (bind _currenttoolactive (Variables|Default|GetCurrentToolActive))
  (bind (_value _returnvalue) (Utilities|Map|Find _toollist _currenttoolactive))
  (if _returnvalue
    (Default|CallEDUseTool _value)
    (Default|CallEDonUseToolManager (Variables|Default|GetCurrentToolActive))))

(fn UseSecondaryTool
  (bind _toollist (Variables|Default|GetToolList))
  (bind _currenttoolactive (Variables|Default|GetCurrentToolActive))
  (bind (_value _returnvalue) (Utilities|Map|Find _toollist _currenttoolactive))
  (if _returnvalue
    (Default|CallEDUseToolSecondaryMode _value)
    (Default|CallEDonUseSecondaryToolManager (Variables|Default|GetCurrentToolActive))))

(fn ToggleTool
  (params (NextTool :type E_ToolShip%20Enum :default "NewEnumerator3"))
  (if (Public|ToolLock|IsLock NextTool)
    (Private|CloseTool (Variables|Default|GetCurrentToolActive) :!label _label)
    (elif (Private|AlreadyActive NextTool)
      (goto _label)
      (else
        (Private|SwitchTool NextTool)))))

(fn SwitchTool
  (params (NewTool :type E_ToolShip%20Enum :default "NewEnumerator0"))
  (Private|CloseTool (Variables|Default|GetCurrentToolActive))
  (Private|OpenTool NewTool))

(fn AlreadyActive
  (params (ToolToActive :type E_ToolShip%20Enum :default "NewEnumerator3"))
  (return (Utilities|Enum|Equal(Enum) ToolToActive (Variables|Default|GetCurrentToolActive))))

(fn AddTool
  (params (Key :type E_ToolShip%20Enum%20%28by%20ref%29 :default "NewEnumerator3") (Value :type BPC%20Tool%20Base%20Object%20Reference%20%28by%20ref%29))
  (Utilities|Map|Add (Variables|Default|GetToolList) Key Value)
  (Default|Initialize Value))

(fn IsLock
  (params (Tool :type E_ToolShip%20Enum%20%28by%20ref%29 :default "NewEnumerator3"))
  (bind _toollist (Variables|Default|GetToolList))
  (bind (_value _returnvalue) (Utilities|Map|Find _toollist Tool))
  (if _returnvalue
    (return (Variables|/Game/Blueprints/Game/Player/ToolsComponent/BPC_ToolBase.BPC_ToolBase_C|GetIsLock _value))))

(fn GetCurrentLevel
  (params (Tool :type E_ToolShip%20Enum :default "NewEnumerator3"))
  (bind _toollist (Variables|Default|GetToolList))
  (bind (_value _returnvalue) (Utilities|Map|Find _toollist Tool))
  (if _returnvalue
    (return (Variables|/Game/Blueprints/Game/Player/ToolsComponent/BPC_ToolBase.BPC_ToolBase_C|GetCurrentLevel _value))))

(fn GetNextLevel
  (params (Tool :type E_ToolShip%20Enum :default "NewEnumerator3") (NextValue :type Integer))
  (bind _toollist (Variables|Default|GetToolList))
  (bind (_value _returnvalue) (Utilities|Map|Find _toollist Tool))
  (if _returnvalue
    (return (Variables|/Game/Blueprints/Game/Player/ToolsComponent/BPC_ToolBase.BPC_ToolBase_C|GetCurrentLevel _value))))

(fn UpgradeTool
  (params (ToolToUpgrade :type E_ToolShip%20Enum%20%28by%20ref%29 :default "NewEnumerator3"))
  (Default|ToolBaseEDUpgradeNextLevel (.Value (Utilities|Map|Find (Variables|Default|GetToolList) ToolToUpgrade)))
  (Default|CallEDonUpgradeToolManager ToolToUpgrade))