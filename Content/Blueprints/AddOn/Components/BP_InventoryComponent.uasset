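; Inventory component that stores caught or collected creature data in an Items map keyed by creature name.
; AddData inserts a new creature or merges a repeat through ModifySettings, which keeps the larger size and weight and sums quantity.
; The updated map then goes to the owning actor through UpdateDataMessage.
; Tick prints every held creature's name as debug text.
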(event EventTick
  (params (DeltaSeconds :type Float%20%28single-precision%29))
  (bind _items (Variables|Default|GetItems))
  (bind _keys (Utilities|Map|Keys _items))
  (for _array_element _keys
    (Development|PrintText (Utilities|Text|FormatText "{n} is in Inventory" (Utilities|String|EnumtoString (.creaturename (.Value (Utilities|Map|Find _items _array_element))))) true true "(R=1.000000,G=0.403349,B=0.000000,A=1.000000)" 0.0)))

(event EventAddData
  (params (Data :type S%20Creature%20Details%20Instanced%20Structure))
  (bind _mapvalue (CallFunction|AddInventory (Variables|Default|GetItems) Data))
  (Class|BPIInventory|UpdateData(Message) (Components|GetOwner) _mapvalue))

(fn ModifySettings
  (params (TargetMap :type Map%20of%20E_CreatureType%20Enums%20to%20Structs :default "NewEnumerator4") (CreatureType :type E_CreatureType%20Enum%20%28by%20ref%29 :default "NewEnumerator4") (Creature%20Stat%20Settings :type S%20AI%20Creature%20Stat%20Settings%20Structure))
  (bind _items (Variables|Default|GetItems))
  (bind _value (Utilities|Map|Find _items CreatureType))
  (Utilities|Map|Add TargetMap CreatureType (Utilities|Struct|MakeS_CreatureDetailsInstanced (.creaturename _value) (.creaturesizetype _value) (Utilities|Struct|MakeS_AICreatureStatSettings (.creaturemesh (.creaturestatsettings _value)) (Math|Float|Max(Float) (.size (.creaturestatsettings _value)) (.size Creature%20Stat%20Settings)) (Math|Float|Max(Float) (.weight (.creaturestatsettings _value)) (.weight Creature%20Stat%20Settings)) (+ (.quantity (.creaturestatsettings _value)) (.quantity Creature%20Stat%20Settings))) (.creaturebehaviorsettings _value)))
  (return))

(fn AddInventory
  (params (TargetMap :type Map%20of%20E_CreatureType%20Enums%20to%20Structs :default "NewEnumerator4") (CreatureDetailsInstanced :type S%20Creature%20Details%20Instanced%20Structure%20%28by%20ref%29))
  (bind (_creaturename _creaturesizetype _creaturestatsettings) (Utilities|Struct|BreakS_CreatureDetailsInstanced CreatureDetailsInstanced))
  (if (.ReturnValue (Utilities|Map|Find TargetMap _creaturename))
    (CallFunction|ModifySettings TargetMap _creaturename _creaturestatsettings)
    (else
      (Utilities|Map|Add TargetMap _creaturename CreatureDetailsInstanced)))
  (return TargetMap))