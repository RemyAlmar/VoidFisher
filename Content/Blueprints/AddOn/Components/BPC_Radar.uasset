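; Radar component that lets the player ping actors and shows screen widgets on the pinned targets.
; A sphere trace along a ray deprojected from the cursor's screen position finds targets, previewed every Tick on a spare widget while pinned widgets update.
; Selection toggles pins on actors with BPC_InformationData, binding or unbinding their OnDestroyed event.
; Pin widgets grow on demand, are reused by index through interface messages, and can be hidden or shown together.
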(event EventTick
  (params (DeltaSeconds :type Float%20%28single-precision%29))
  (Private|PreshowTarget (Public|Get|GetPreshowPin))
  (for _index (range 0 (Utilities|Array|LastIndex (Variables|Param|GetCurrentTargetPinned)))
    (Class|BPITargetable|IShowTarget(Message) (Utilities|Array|Get(acopy) (Variables|Param|GetPinWidget) _index))))

(fn GetTargetLocationHit
  (params (Start :type Vector) (Direction :type Vector))
  (bind _outhit (Collision|SphereTraceByChannel Start (+ Start (* Direction (Variables|Default|GetDistanceDetect))) 3e+02 "TraceTypeQuery1" false 0 "None"))
  (LocalVariables|SetHasHit (.bBlockingHit (Collision|BreakHitResult _outhit)))
  (bind _output_get (LocalVariables|SetTarget (.HitActor (Collision|BreakHitResult _outhit))))
  (return (LocalVariables|GetHasHit) _output_get))

(fn DisplayWidgetonTarget
  (bind _targetout (Private|GetTargetLocationHit (Variables|Default|GetRadarPosition) (Variables|Default|GetRadarDirection)))
  (Public|Set|SetCurrentTarget _targetout))

(fn SetDataforRaycast
  (params (CursorLocation :type Vector))
  (bind _returnvalue (Game|GetPlayerController 0))
  (bind _screenposition (Class|GameplayStatics|ProjectWorldtoScreen _returnvalue CursorLocation false))
  (bind (_worldposition _worlddirection) (Class|GameplayStatics|DeprojectScreentoWorld _returnvalue _screenposition))
  (Variables|Default|SetRadarDirection _worlddirection)
  (Variables|Default|SetRadarPosition _worldposition))

(fn IsNotPinned
  (params (ItemToFind :type Actor%20Object%20Reference%20%28by%20ref%29))
  (return (not (Utilities|Array|ContainsItem (Variables|Param|GetCurrentTargetPinned) ItemToFind))))

(fn PreshowTarget
  (params (PinTarget :type Object%20Object%20Reference))
  (bind _targetout (Private|GetTargetLocationHit (Variables|Default|GetRadarPosition) (Variables|Default|GetRadarDirection)))
  (if (Public||IsNotPinned _targetout)
    (LocalVariables|SetTarget _targetout))
  (Class|BPITargetable|IPreShowTarget(Message) PinTarget (LocalVariables|GetTarget)))

(fn CreatePinWidget
  (bind _returnvalue (UserInterface|CreateWidget (Variables|Param|GetWidgetClass)))
  (Utilities|Array|Add (Variables|Param|GetPinWidget) _returnvalue)
  (UserInterface|Viewport|AddtoViewport _returnvalue -1)
  (return))

(fn GetCurrentMaxTarget
  (return (+ (Utilities|Array|LastIndex (Variables|Param|GetCurrentTargetPinned)) 1)))

(fn GetPreshowPin
  (bind _pinwidget (Variables|Param|GetPinWidget))
  (bind _returnvalue (Utilities|Array|LastIndex _pinwidget))
  (bind _output_get (LocalVariables|SetLastIndex (Public|get|GetCurrentMaxTarget)))
  (if (< _returnvalue _output_get)
    (Private|CreatePinWidget)
    (LocalVariables|SetLastIndex _returnvalue))
  (return (Utilities|Array|Get(acopy) (Variables|Param|GetPinWidget) (LocalVariables|GetLastIndex))))

(fn ClearUnusedPin
  (Public||RefreshActorPinned)
  (for _index (range (Public|get|GetCurrentMaxTarget) (Utilities|Array|LastIndex (Variables|Param|GetPinWidget)))
    (Class|BPITargetable|ISetTarget(Message) (Utilities|Array|Get(acopy) (Variables|Param|GetPinWidget) _index)))
  (return))

(fn RefreshActorPinned
  (for (_array_element _array_index) (Variables|Param|GetCurrentTargetPinned)
    (Class|BPITargetable|IResetTarget(Message) (Utilities|Array|Get(acopy) (Variables|Param|GetPinWidget) _array_index) _array_element))
  (return))

(fn SetCurrentTarget
  (params (Target :type Actor%20Object%20Reference))
  (bind _currenttargetpinned (Variables|Param|GetCurrentTargetPinned))
  (bind _output_get (LocalVariables|SetCurrentTarget Target))
  (Utilities|IsValid _output_get
    (:Is%20Valid
      (Utilities|IsValid (Actor|GetComponentbyClass (LocalVariables|GetCurrentTarget) "/Game/Blueprints/AddOn/Components/BPC_InformationData.BPC_InformationData_C")
        (:Is%20Valid
          (if (Utilities|Array|ContainsItem _currenttargetpinned (LocalVariables|GetCurrentTarget))
            (LocalVariables|SetIndexItem (Utilities|Array|FindItem _currenttargetpinned (LocalVariables|GetCurrentTarget)))
            (Utilities|Array|RemoveItem _currenttargetpinned (LocalVariables|GetCurrentTarget))
            (Game|UnbindEventfromOnDestroyed (LocalVariables|GetCurrentTarget) (EventDispatchers|CreateEvent :!event SetCurrentTarget))
            (else
              (bind _returnvalue (Utilities|Array|Add _currenttargetpinned (LocalVariables|GetCurrentTarget)))
              (LocalVariables|SetIndexItem _returnvalue)
              (Game|BindEventtoOnDestroyed (LocalVariables|GetCurrentTarget) (EventDispatchers|CreateEvent :!event SetCurrentTarget))))
          (Class|BPITargetable|ISetTarget(Message) (Utilities|Array|Get(acopy) (Variables|Param|GetPinWidget) (LocalVariables|GetIndexItem)) (LocalVariables|GetCurrentTarget))
          (Public||ClearUnusedPin))))))

(fn ClearAllPings
  (bind _currenttargetpinned (Variables|Param|GetCurrentTargetPinned))
  (for _array_element _currenttargetpinned
    (Public|Set|SetCurrentTarget _array_element))
  (Utilities|Array|Clear _currenttargetpinned))

(fn HideAllPings
  (for _array_element (Variables|Param|GetPinWidget)
    (Widget|SetVisibility _array_element "Collapsed")))

(fn ShowAllPings
  (for _array_element (Variables|Param|GetPinWidget)
    (Widget|SetVisibility _array_element "SelfHitTestInvisible")))