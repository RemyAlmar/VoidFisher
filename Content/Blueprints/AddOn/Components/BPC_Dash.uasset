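; Dash add-on component that gives a physics-movement actor a forward dash when its active-tool event fires and dashing is available.
; Dash power is a percentage of the movement component's max speed, applied along the root's forward vector as an extra force and target direction.
; A state commander, created on BeginPlay and updated each tick, runs the dash states, with event dispatchers signalling init, use and availability.
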(event EventBeginPlay
  (bind _asbpc_actor_physics_movement (Utilities|Casting|CastToBPC_ActorPhysicsMovement (CallFunction|GetComponentInstance (Components|GetOwner) "/Game/Blueprints/AddOn/Components/BPC_ActorPhysicsMovement.BPC_ActorPhysicsMovement_C")))
  (Variables|Default|SetBPC_PhysicsMovement _asbpc_actor_physics_movement)
  (CallFunction|ResetDashPower)
  (bind _returnvalue (Game|ConstructObjectfromClass "/Game/Blueprints/AI/StateMachine/BP_StateCommander.BP_StateCommander_C"))
  (bind _output_get (Variables|StateMachine|Commander|SetStateCommander _returnvalue))
  (Default|InititalizeCommander _output_get (Components|GetOwner) (Variables|StateMachine|GetList%20States%20Class))
  (Default|CallEDonInit)
  (|CallParentFunction))

(event EventEDActiveToolEvent
  (|CallParentFunction)
  (CallFunction|UseDashHandle))

(event EventTick
  (params (DeltaSeconds :type Float%20%28single-precision%29))
  (bind _statecommander (Variables|StateMachine|Commander|GetStateCommander)
    (:then
      (Default|IUpdate _statecommander DeltaSeconds))
    (:else)))

(fn ResetDashPower
  (Variables|Stat|SetDashPower (* (Variables|/Game/Blueprints/AddOn/Components/BPC_ActorPhysicsMovement.BPC_ActorPhysicsMovement_C|GetMaxSpeed (Variables|Default|GetBPC_PhysicsMovement)) (/ (Variables|Stat|GetPowerPercent) 1e+02))))

(fn SetDashForce
  (Variables|Stat|SetDashForce (* (Math|Vector|GetForwardVector (Variables|/Game/Blueprints/AddOn/Components/BPC_ActorPhysicsMovement.BPC_ActorPhysicsMovement_C|GetOwnRootPhysics (Variables|Default|GetBPC_PhysicsMovement))) (Variables|Stat|GetDashPower))))

(fn ApplyDashForce
  (bind _bpc_physicsmovement (Variables|Default|GetBPC_PhysicsMovement))
  (bind _dashforce (Variables|Stat|GetDashForce))
  (Default|SetOtherForcesMovement _bpc_physicsmovement _dashforce)
  (Variables|/Game/Blueprints/AddOn/Components/BPC_ActorPhysicsMovement.BPC_ActorPhysicsMovement_C|SetTargetDirection _bpc_physicsmovement (Math|Vector|Normalize _dashforce)))

(fn UseDashHandle
  (if (Variables|StateMachine|GetCanDash)
    (Default|CallEDUseDashHandle) ; Est appelé dans le state Use Dash
    (return)))

(fn SetCanDash
  (params (CanDash :type Boolean))
  (LocalVariables|SetPreviousValue (Variables|StateMachine|GetCanDash))
  (Variables|StateMachine|SetCanDash CanDash)
  (if (!= (Variables|StateMachine|GetCanDash) (LocalVariables|GetPreviousValue))
    (Default|CallEDonDashAvailable (Variables|StateMachine|GetCanDash))))

(fn StopDashForce
  (Variables|Stat|SetDashForce "0, 0, 0"))