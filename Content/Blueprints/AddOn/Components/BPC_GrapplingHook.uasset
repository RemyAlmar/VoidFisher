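; Grappling hook component that attaches its owner's primitive root to an anchor component and detaches it on release.
; On hook, it attaches with rules based on anchor physics, spawns an impact Niagara effect, then teleports to the target relative transform next tick.
; Event dispatchers relay hook, release, pull strength and physics changes; SetSimulatePhysics only signals state changes, without setting physics itself.
; Tick is enabled while hooked to broadcast the hooked state.
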(event Custom|ED_AddHookOnAnchor_Event
  (params (TargetAnchor :type Scene%20Component%20Object%20Reference) (TargetLocation :type Vector) (TargetRotation :type Rotator))
  ;[1 0.75 0] Accroche le grappin à l'Ancre
  (if (Variables|Default|GetCanHook)
    (Variables|Default|SetTargetLocation TargetLocation)
    (Variables|Default|SetTargetRotation TargetRotation)
    (bind (_newparent _returnvalue) (CallFunction|AttachOwnerActor TargetAnchor))
    (if _returnvalue
      (bind _output_get (Variables|AnchorImpact|SetTarget%20Anchor _newparent))
      (Default|CallEDAddHookonAnchor _output_get (Variables|Default|GetTargetLocation) (Variables|Default|GetTargetRotation))
      (Niagara|SpawnSystematLocation "/Game/VFX/Niagara/Player/NS_ShipColision.NS_ShipColision" (Variables|Default|GetTargetLocation) (Variables|Default|GetTargetRotation))
      (CallFunction|EDHookonAnchorEvent)
      (else
        (CallFunction|EDRemoveHookonAnchorEvent)
        (Development|PrintText "Watf ca pete tout" true true "(R=0.282040,G=1.000000,B=0.110609,A=1.000000)" 1e+01)))))

(event Custom|ED_RemoveHookOnAnchor_Event
  ;[1 0.3154 0] Se retire de l'ancre
  (if (not (Variables|Default|GetCanHook))
    (Variables|AnchorImpact|GetTarget%20Anchor
      (:then
        (Transformation|DetachFromComponent (Variables|Default|GetRoot) "KeepWorld" "KeepWorld" "KeepWorld" false)
        (Variables|AnchorImpact|SetTarget%20Anchor 0)
        (CallFunction|SetSimulatePhysics true)
        (bind _output_get (Variables|Default|SetHooked false))
        (Components|Tick|SetComponentTickEnabled _output_get)
        (Default|CallEDRemoveHookonAnchor))
      (:else
        (bind _output_get_2 (Variables|Default|SetHooked false))
        (Components|Tick|SetComponentTickEnabled _output_get_2)))))

(event Custom|ED_OnPhysicsDeactivated_Event
  (Default|CallEDonPhysicsDeactivated))

(event Custom|ED_OnAnchorPhysicsChanged_Event
  (params (CurrentPhysics :type Boolean))
  ;[0.469 1 0] Event appelé quand physique de l'ancre actuelle change
  (Default|CallEDonAnchorPhysicsChanged CurrentPhysics)
  (CallFunction|SetSimulatePhysics CurrentPhysics)
  (Development|PrintText (Utilities|Text|FormatText "Become Physiqued {x}" (Physics|IsSimulatingPhysics (Variables|Default|GetRoot) "None")) true true "(R=1.000000,G=0.000000,B=0.135502,A=1.000000)" 5.0))

(event Custom|ED_HookOnAnchor_Event
  (bind _returnvalue (Components|GetOwner))
  ;[1 0.5143 0.0245] Est accroché à l'ancre
  (Utilities|FlowControl|DelayUntilNextTick)
  (Transformation|SetActorRelativeLocation _returnvalue (Variables|Default|GetTargetLocation) false true)
  (Transformation|SetActorRelativeRotation _returnvalue (Variables|Default|GetTargetRotation) false true)
  (Variables|Default|SetCanHook false)
  (bind _output_get (Variables|Default|SetHooked true))
  (Components|Tick|SetComponentTickEnabled _output_get)
  (Default|CallEDHookonAnchor))

(event Custom|ED_CurrentlyHooked_Event
  (Default|CallEDCurrentlyHooked))

(event Custom|ED_PullStrength_Event
  (params (Strength :type Float%20%28double-precision%29) (TensionDirection :type Vector))
  ;[0.469 1 0] Event appelé quand physique de l'ancre actuelle change
  (Default|CallEDPullStrength Strength TensionDirection))

(event Custom|ED_OnPhysicsChanged_Event
  (params (CurrentPhysics :type Boolean))
  (Default|CallEDonPhysicsChanged CurrentPhysics))

(event Custom|ED_OnPhysicsActivated_Event
  (Default|CallEDonPhysicsActivated))

(event EventTick
  (params (DeltaSeconds :type Float%20%28single-precision%29))
  (if (Variables|Default|GetHooked)
    (CallFunction|EDCurrentlyHookedEvent)))

(event EventBeginPlay
  (bind _returnvalue (Components|GetOwner))
  (bind _asprimitive_component (Utilities|Casting|CastToPrimitiveComponent (Variables|/Script/Engine.Actor|GetRootComponent _returnvalue))
    (:then
      (Variables|Default|SetRoot _asprimitive_component))
    (:CastFailed
      (Development|PrintText (Utilities|Text|FormatText "{x} has not a primitive component as root" (Utilities|GetDisplayName _returnvalue)) true true "(R=1.000000,G=0.000000,B=0.045438,A=1.000000)" 15.0))))

(fn AttachOwnerActor
  (params (Parent :type Scene%20Component%20Object%20Reference))
  (CallFunction|SetSimulatePhysics false)
  (if (Physics|IsSimulatingPhysics Parent "None")
    (LocalVariables|SetAttachementRule "KeepWorld")
    (else
      (LocalVariables|SetAttachementRule "KeepRelative")))
  (bind _returnvalue (Transformation|AttachComponentToComponent (Variables|Default|GetRoot) Parent "None" (LocalVariables|GetAttachementRule) (LocalVariables|GetAttachementRule) "KeepWorld" false))
  (return Parent _returnvalue))

(fn SetPullStrength
  (params (StrengthTension :type Float%20%28double-precision%29) (TensionDirection :type Vector))
  (bind _output_get (Variables|Default|SetStrength%20Tension StrengthTension))
  (CallFunction|EDPullStrengthEvent _output_get TensionDirection))

(fn SetSimulatePhysics
  (params (SimulatePhysics :type Boolean))
  (LocalVariables|SetPreviousValue (Physics|IsSimulatingPhysics (Variables|Default|GetRoot) "None"))
  (if (!= (LocalVariables|GetPreviousValue) SimulatePhysics) ; Si valeur inchangée
    (CallFunction|EDonPhysicsChangedEvent SimulatePhysics)
    (if SimulatePhysics
      (CallFunction|EDonPhysicsActivatedEvent)
      (else
        (CallFunction|EDonPhysicsDeactivatedEvent)))))