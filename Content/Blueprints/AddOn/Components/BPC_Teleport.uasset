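; Player component that implements a hold-to-charge teleport to the first TargetPoint tagged "Teleport".
; Started spawns an attached Niagara effect, and Canceled destroys it and resets the charge.
; Each Teleport call adds frame time until MaintainTime, then widens the camera FOV, moves the owner and restarts the cooldown.
; Tick advances the cooldown, whose Cooldown flag is true when teleporting is available.
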(event EventBeginPlay
  (bind _outactors (Actor|GetAllActorsOfClasswithTag "/Script/Engine.TargetPoint" "Teleport"))
  (Variables|Default|SetTeleport%20Point (Utilities|Array|Get(acopy) _outactors))
  (bind _asbp_player_refonte (Utilities|Casting|CastToBP_PlayerRefonte (Components|GetOwner)))
  (Variables|Default|SetCamera (Variables|/Game/Blueprints/Game/Player/Controllers/BP_PlayerRefonte.BP_PlayerRefonte_C|GetCamera _asbp_player_refonte)))

(event EventTick
  (params (DeltaSeconds :type Float%20%28single-precision%29))
  (Utilities|FlowControl|Sequence
    (:then_0
      (if (Variables|Default|GetHaveToDecrease)
        (Variables|Default|SetCurrentTime (Math|Interpolation|FInterptoConstant (Variables|Default|GetCurrentTime) 0.0 0.0 0.1))))
    (:then_1
      (bind _output_get (Variables|Default|SetCurrentCooldown (+ (Variables|Default|GetCurrentCooldown) DeltaSeconds)))
      (Variables|Default|SetCooldown (> _output_get (Variables|Default|GetCooldownTime))))))

(fn Teleport
  (if (Variables|Default|GetCooldown)
    (Variables|Default|SetCurrentTime (Math|Float|Clamp(Float) (+ (Utilities|Time|GetWorldDeltaSeconds) (Variables|Default|GetCurrentTime)) 0.0 (Variables|Skills|GetMaintainTime)))
    (if (>= (Variables|Default|GetCurrentTime) (Variables|Skills|GetMaintainTime))
      (Camera|SetFieldOfView (Variables|Default|GetCamera) 2.6e+02)
      (Transformation|SetActorTransform (Components|GetOwner) (Transformation|GetActorTransform (Variables|Default|GetTeleport%20Point)) false true)
      (CallFunction|Canceled)
      (Variables|Default|SetCooldown false)
      (Variables|Default|SetCurrentCooldown 0.0)
      (return true)
      (else
        (Variables|Default|SetHaveToDecrease (not (>= (Variables|Default|GetCurrentTime) (Variables|Skills|GetMaintainTime))))
        (return false)))
    (else
      (return false))))

(fn Canceled
  (Variables|Default|SetCurrentTime 0.0)
  (bind _niagara (Variables|Default|GetNiagara)
    (:then
      (Components|DestroyComponent _niagara))
    (:else)))

(fn Started
  (if (Variables|Default|GetCooldown)
    (bind _returnvalue (Niagara|SpawnSystemAttached "/Game/VFX/Niagara/Player/NS_Teleport.NS_Teleport" (Variables|/Script/Engine.Actor|GetRootComponent (Components|GetOwner)) "Root" "0, 0, 0" "0, 0, 0" "KeepRelativeOffset" true))
    (Variables|Default|SetNiagara _returnvalue)))