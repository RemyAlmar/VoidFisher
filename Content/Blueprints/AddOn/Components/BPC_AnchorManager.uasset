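; Component that turns its owner into a grappling hook target for actors carrying BPC_GrapplingHook.
; On BeginPlay it spawns overlap spheres with Niagara markers on the skeletal mesh's "Anchor" sockets, or falls back to root primitive hits if none exist.
; Contact places an arrow as anchor point, notifies the hook and relays attach, detach, pull and physics changes through dispatchers.
; A sphere-to-bool map drives anchor activation, overlap and visibility.
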(event Custom|PrimitiveComponent_OnHit
  (params (HitComponent :type Primitive%20Component%20Object%20Reference) (OtherActor :type Actor%20Object%20Reference) (OtherComp :type Primitive%20Component%20Object%20Reference) (NormalImpulse :type Vector) (Hit :type Hit%20Result%20Structure%20%28by%20ref%29))
  (bind _returnvalue (Actor|GetComponentbyClass OtherActor "/Game/Blueprints/AddOn/Components/BPC_GrapplingHook.BPC_GrapplingHook_C"))
  (bind (_bblockinghit _binitialoverlap _time _distance _location _impactpoint _normal _impactnormal) (Collision|BreakHitResult Hit))
  (Utilities|IsValid _returnvalue
    (:Is%20Valid
      (Variables|Default|SetHookComp _returnvalue)
      (Creation|CreateAnchorPoint HitComponent OtherActor _impactpoint _impactnormal))))

(event Custom|SphereCollision_OnOverlapEvent
  (params (OverlappedComponent :type Primitive%20Component%20Object%20Reference) (OtherActor :type Actor%20Object%20Reference) (OtherComp :type Primitive%20Component%20Object%20Reference) (OtherBodyIndex :type Integer) (bFromSweep :type Boolean) (SweepResult :type Hit%20Result%20Structure%20%28by%20ref%29))
  (bind _returnvalue (Actor|GetComponentbyClass OtherActor "/Game/Blueprints/AddOn/Components/BPC_GrapplingHook.BPC_GrapplingHook_C"))
  (Utilities|IsValid _returnvalue
    (:Is%20Valid
      (Variables|Default|SetHookComp _returnvalue)
      (HandleAnchor|SetCurrentAnchorHooked OverlappedComponent)
      (Creation|CreateAnchorPoint OverlappedComponent OtherActor "0, 0, 0" "0, 0, 0"))))

(event Custom|ED_OnPhysicsDeactivated_Event
  (Default|CallEDonPhysicsDeactivated))

(event Custom|Hook_ED_PullStrength_Event
  (params (Strength :type Float%20%28double-precision%29) (TensionDirection :type Vector))
  (Default|CallEDonHookPulled Strength TensionDirection))

(event Custom|ED_OnAttachHook_Event
  (Default|CallEDonAttachHook)
  (EventDispatchers|BindEventtoEDPullStrength (Variables|Default|GetHookComp) (EventDispatchers|CreateEvent :!event Custom|Hook_ED_PullStrength_Event)))

(event Custom|BPC_GrapHook_ED_OnDetachHook_Event
  ;[1 0.4722 0] Retire l'ancre des reference et retire l'abonnement des events dispatcher
  (bind _hookcomp (Variables|Default|GetHookComp)
    (:then
      (CallFunction|EDonDetachHookEvent)
      (EventDispatchers|UnbindEventfromEDHookonAnchor _hookcomp (EventDispatchers|CreateEvent :!event Custom|BPC_GrapHook_ED_OnAttachHook_Event))
      (EventDispatchers|UnbindEventfromEDonPhysicsChanged (EventDispatchers|CreateEvent _hookcomp :!event Custom|ED_OnPhysicsChanged_Event))
      (EventDispatchers|UnbindEventfromEDPullStrength (Variables|Default|GetHookComp) (EventDispatchers|CreateEvent :!event Custom|Hook_ED_PullStrength_Event))
      (Variables|Default|SetHookComp 0))
    (:else)))

(event Custom|BPC_GrapHook_ED_OnAttachHook_Event
  (CallFunction|EDonAttachHookEvent))

(event Custom|OnComponentActivate
  (params (Active :type Boolean))
  (HandleAnchor|ActiveAllAnchors Active))

(event Custom|ED_OnDetachHook_Event
  (Default|CallEDonDetachHook))

(event Custom|ED_OnPhysicsChanged_Event
  (params (SimulatePhysics :type Boolean))
  (Default|CallEDonPhysicsChanged SimulatePhysics))

(event Custom|ED_OnPhysicsActivated_Event
  (Default|CallEDonPhysicsActivated))

(event EventBeginPlay
  (bind _returnvalue (Components|GetOwner))
  (bind _returnvalue_2 (Actor|GetComponentbyClass _returnvalue "/Script/Engine.SkeletalMeshComponent"))
  (bind _asprimitive_component (Utilities|Casting|CastToPrimitiveComponent (Variables|/Script/Engine.Actor|GetRootComponent _returnvalue)))
  (Variables|Default|SetParentMesh _asprimitive_component)
  (Utilities|IsValid _returnvalue_2
    (:Is%20Valid
      (Variables|Default|SetSocketsAnchor (CallFunction|GetSocketName "Anchor" (Transformation|GetAllSocketNames _returnvalue_2)))
      (if (Utilities|Array|IsEmpty (Variables|Default|GetSocketsAnchor))
        _
        (else
          (Variables|Default|SetParentMesh _returnvalue_2))))
    (:Is%20Not%20Valid
      _))
  (Variables|Default|SetMesh%20Is%20Collider (Utilities|Array|IsEmpty (Variables|Default|GetSocketsAnchor)))
  (Initialization|Initialize (Variables|Default|GetMesh%20Is%20Collider) (Variables|Default|GetParentMesh) 1.0 (Variables|Default|GetSocketsAnchor)))

(fn Initialize
  (params (MeshIsCollider :type Boolean) (TargetParent :type Scene%20Component%20Object%20Reference) (AnchorRadius :type Float%20%28double-precision%29) (SocketList :type Array%20of%20Names))
  (bind _output_get (Variables|Default|SetMesh%20Is%20Collider MeshIsCollider))
  (if _output_get
    (Collision|BindEventtoOnComponentHit (Variables|Default|GetParentMesh) (EventDispatchers|CreateEvent :!event Custom|PrimitiveComponent_OnHit))
    (else
      (Variables|SphereCollision|Radius|SetAnchorRadiusCurrent (* AnchorRadius (Variables|SphereCollision|Radius|GetAnchorRadiusBase)))
      (if (Utilities|Array|IsNotEmpty SocketList)
        (for _array_element SocketList
          (Creation|CreateAnchor TargetParent (Variables|SphereCollision|Radius|GetAnchorRadiusCurrent) _array_element))
        (else
          (Creation|CreateAnchor TargetParent (Variables|SphereCollision|Radius|GetAnchorRadiusCurrent) "None")))))
  (return))

(fn CreateAnchor
  (params (Parent :type Scene%20Component%20Object%20Reference%20%28by%20ref%29) (RadiusMultiplier :type Float%20%28double-precision%29) (SocketName :type Name :default "None"))
  (bind _returnvalue (Game|AddComponentbyClass (Components|GetOwner) "/Script/Engine.SphereComponent" true))
  (bind _output_get (LocalVariables|Setlocal_SphereColl _returnvalue))
  (Transformation|AttachComponentToComponent _output_get Parent SocketName (Variables|SphereCollision|TransformRules|GetSphereCollision_Location%20Rule) (Variables|SphereCollision|TransformRules|GetSphereCollision_Rotation%20Rule) (Variables|SphereCollision|TransformRules|GetSphereCollision_Scale%20Rule) false)
  (Components|Sphere|SetSphereRadius _output_get RadiusMultiplier true)
  (Collision|SetCollisionProfileName (LocalVariables|Getlocal_SphereColl) (Variables|SphereCollision|Collision|GetCollisionPresetName) true :!class /Script/Engine.PrimitiveComponent)
  (Variables|/Script/Engine.PrimitiveComponent|SetbGenerateOverlapEvents (LocalVariables|Getlocal_SphereColl) true)
  (Rendering|SetVisibility (LocalVariables|Getlocal_SphereColl) (Variables|SphereCollision|Visibility|GetSphereCollision_Visibility) false)
  (Development|SetHiddeninGame (LocalVariables|Getlocal_SphereColl) (Variables|SphereCollision|Visibility|GetSphereCollision_HiddenInGame) false)
  (Collision|BindEventtoOnComponentBeginOverlap (LocalVariables|Getlocal_SphereColl) (EventDispatchers|CreateEvent :!event Custom|SphereCollision_OnOverlapEvent))
  (Utilities|Map|Add (Variables|Default|GetAnchorList) (LocalVariables|Getlocal_SphereColl) true)
  (bind _returnvalue_2 (Niagara|SpawnSystemAttached "/Game/VFX/Niagara/Fish/NS_Anchor.NS_Anchor" (LocalVariables|Getlocal_SphereColl) SocketName "0, 0, 0" "0, 0, 0" "SnapToTargetIncludingScale" false))
  (Utilities|Array|SetArrayElem (Variables|Default|GetNS_Anchor) (CallFunction|GetAnchorIndex (LocalVariables|Getlocal_SphereColl)) _returnvalue_2 true)
  (return))

(fn CreateAnchorPoint
  (params (TargetComponent :type Scene%20Component%20Object%20Reference%20%28by%20ref%29) (TargetActor :type Actor%20Object%20Reference) (ImpactLocation :type Vector) (ImpactDirection :type Vector))
  (bind _hookcomp (Variables|Default|GetHookComp))
  (EventDispatchers|BindEventtoEDHookonAnchor _hookcomp (EventDispatchers|CreateEvent :!event Custom|BPC_GrapHook_ED_OnAttachHook_Event))
  (EventDispatchers|BindEventtoEDRemoveHookonAnchor _hookcomp (EventDispatchers|CreateEvent :!event Custom|BPC_GrapHook_ED_OnDetachHook_Event))
  (EventDispatchers|BindEventtoEDonPhysicsChanged (EventDispatchers|CreateEvent _hookcomp :!event EDonAnchorPhysicsChangedEvent))
  (if (Variables|Default|GetMesh%20Is%20Collider)
    (LocalVariables|SetArrowDir ImpactDirection)
    (LocalVariables|SetImpactWorldLocation (Math|Transform|InverseTransformLocation (Transformation|GetWorldTransform TargetComponent) ImpactLocation))
    (LocalVariables|SetRotationToDirection (Math|Conversions|RotationFromXVector (LocalVariables|GetArrowDir))))
  (Default|EDAddHookonAnchorEvent (Variables|Default|GetHookComp) TargetComponent (LocalVariables|GetImpactWorldLocation) (LocalVariables|GetRotationToDirection))
  (Creation|CreateArrow TargetComponent (LocalVariables|GetImpactWorldLocation) (LocalVariables|GetRotationToDirection))
  (CallFunction|SetAnchorsIsActive true))

(fn SetCurrentAnchorHooked
  (params (Object :type Object%20Object%20Reference))
  (bind _assphere_collision (Utilities|Casting|CastToSphereComponent Object))
  (if (Utilities|Map|Contains (Variables|Default|GetAnchorList) _assphere_collision)
    (Variables|Default|SetCurrentAnchorHooked _assphere_collision)
    (return)))

(fn GetAnchorHooked
  (if (Variables|Default|GetMesh%20Is%20Collider)
    (LocalVariables|SetCurrentAnchor (Variables|Default|GetParentMesh))
    (else
      (LocalVariables|SetCurrentAnchor (Variables|Default|GetCurrentAnchorHooked))))
  (return (LocalVariables|GetCurrentAnchor)))

(fn RemoveAnchor
  (params (Item :type Sphere%20Component%20Object%20Reference%20%28by%20ref%29))
  (Utilities|IsValid Item
    (:Is%20Valid
      (Collision|UnbindEventfromOnComponentBeginOverlap Item (EventDispatchers|CreateEvent :!event Custom|SphereCollision_OnOverlapEvent))
      (HandleAnchor|ActiveAnchor Item false)
      (return))))

(fn GetSphereAnchorHooked
  (return (Variables|Default|GetCurrentAnchorHooked)))

(fn CreateArrow
  (params (TargetComponent :type Scene%20Component%20Object%20Reference%20%28by%20ref%29) (ArrowLocationRel :type Vector) (Rotation :type Rotator))
  (bind _anchorpoint (Variables|Default|GetAnchorPoint)
    (:then
      (Components|DestroyComponent _anchorpoint))
    (:else
      _))
  (bind _returnvalue (Game|AddComponentbyClass (Components|GetOwner) "/Script/Engine.ArrowComponent" true (Math|Transform|MakeTransform ArrowLocationRel Rotation "1.000000,1.000000,1.000000")))
  (bind _output_get (Variables|Default|SetAnchorPoint _returnvalue))
  (Variables|/Script/Engine.ArrowComponent|SetArrowSize _output_get 1.0)
  (Transformation|AttachComponentToComponent (Variables|Default|GetAnchorPoint) TargetComponent "None" (Variables|Arrow|TransformRules|GetArrow_Location%20Rule) (Variables|Arrow|TransformRules|GetArrow_Rotation%20Rule) (Variables|Arrow|TransformRules|GetArrow_Scale%20Rule) false)
  (Development|SetHiddeninGame (Variables|Default|GetAnchorPoint) (Variables|Arrow|Visibility|GetAnchorPoint_HiddenInGame) false)
  (Rendering|SetVisibility (Variables|Default|GetAnchorPoint) false false)
  (return))

(fn ActiveAnchor
  (params (Target :type Sphere%20Component%20Object%20Reference%20%28by%20ref%29) (Value :type Boolean))
  (Utilities|Map|Add (Variables|Default|GetAnchorList) Target Value)
  (bind _output_get (Variables|/Script/Engine.PrimitiveComponent|SetbGenerateOverlapEvents Target Value))
  (CallFunction|SetRenderActiveNSbyAnchor Target _output_get)
  (if (.Value (Utilities|Map|Find (Variables|Default|GetAnchorList) Target))
    _
    (else
      (bind _hookcomp (Variables|Default|GetHookComp)
        (:then
          (Default|EDRemoveHookonAnchorEvent _hookcomp))
        (:else))))
  (return))

(fn ResetAllAnchor
  (bind _keys (Utilities|Map|Keys (Variables|Default|GetAnchorList)))
  (for _array_element _keys
    (Utilities|Map|Add (Variables|Default|GetAnchorList) _array_element true))
  (return))

(fn HasAnchorActive
  (bind _keys (Utilities|Map|Keys (Variables|Default|GetAnchorList)))
  (for _array_element _keys
    (if (.Value (Utilities|Map|Find (Variables|Default|GetAnchorList) _array_element))
      (Math|Integer|IncrementInt (LocalVariables|GetNumberActif)
        (:%20%20
          (LocalVariables|SetIsActive true)))))
  (return (LocalVariables|GetIsActive) (LocalVariables|GetNumberActif)))

(fn ActiveAllAnchors
  (params (Active :type Boolean))
  (bind _keys (Utilities|Map|Keys (Variables|Default|GetAnchorList)))
  (for _array_element _keys
    (Variables|/Script/Engine.PrimitiveComponent|SetbGenerateOverlapEvents _array_element (and (.Value (Utilities|Map|Find (Variables|Default|GetAnchorList) _array_element)) Active))
    (Components|Activation|SetActive _array_element (and (.Value (Utilities|Map|Find (Variables|Default|GetAnchorList) _array_element)) Active) false)
    (Rendering|SetVisibility _array_element (and (.Value (Utilities|Map|Find (Variables|Default|GetAnchorList) _array_element)) Active) false))
  (return))

(fn SetSimulatePhysics
  (params (SimulatePhysics :type Boolean))
  (LocalVariables|SetPreviousValue (Physics|IsSimulatingPhysics (Variables|Default|GetParentMesh) "None"))
  (if (not (== (LocalVariables|GetPreviousValue) SimulatePhysics))
    (Physics|SetSimulatePhysics (Variables|Default|GetParentMesh) SimulatePhysics)
    (CallFunction|EDonPhysicsChangedEvent SimulatePhysics)
    (if SimulatePhysics
      (CallFunction|EDonPhysicsActivatedEvent)
      (else
        (CallFunction|EDonPhysicsDeactivatedEvent)))))

(fn SetAnchorRadius
  (params (InSphereRadius :type Float%20%28single-precision%29))
  (Variables|SphereCollision|Radius|SetAnchorRadiusCurrent InSphereRadius)
  (bind _keys (Utilities|Map|Keys (Variables|Default|GetAnchorList)))
  (for _array_element _keys
    (Components|Sphere|SetSphereRadius _array_element (Variables|SphereCollision|Radius|GetAnchorRadiusCurrent) true))
  (return))

(fn ActiveOverlapAnchor
  (params (Target :type Sphere%20Component%20Object%20Reference%20%28by%20ref%29) (Value :type Boolean))
  (if (.Value (Utilities|Map|Find (Variables|Default|GetAnchorList) Target))
    (bind _output_get (Variables|/Script/Engine.PrimitiveComponent|SetbGenerateOverlapEvents Target Value))
    (CallFunction|SetRenderActiveNSbyAnchor Target _output_get)
    (if _output_get
      _
      (else
        (bind _hookcomp (Variables|Default|GetHookComp)
          (:then
            (Default|EDRemoveHookonAnchorEvent _hookcomp))
          (:else))))
    (return)))

(fn ActiveAllOverlapAnchors
  (params (Active :type Boolean))
  (bind _keys (Utilities|Map|Keys (Variables|Default|GetAnchorList)))
  (for _array_element _keys
    (HandleAnchor|ActiveOverlapAnchor _array_element Active))
  (return))

(fn DisplayAnchorsInactive
  (params (Hidden :type Boolean))
  (LocalVariables|SetIsHidden Hidden)
  (bind _keys (Utilities|Map|Keys (Variables|Default|GetAnchorList)))
  (for _array_element _keys
    (if Hidden
      _
      (else
        (LocalVariables|SetIsHidden (.Value (Utilities|Map|Find (Variables|Default|GetAnchorList) _array_element)))))
    (Development|SetHiddeninGame _array_element (LocalVariables|GetIsHidden) false)))

(fn DisplayAnchors
  (params (Hidden :type Boolean))
  (bind _keys (Utilities|Map|Keys (Variables|Default|GetAnchorList)))
  (for _array_element _keys
    (Development|SetHiddeninGame _array_element Hidden false))
  (return))

(fn SetAnchorsIsActive
  (params (CurrentValue :type Boolean))
  (LocalVariables|SetPreviousValue (Variables|Default|GetAnchorsIsActive))
  (Variables|Default|SetAnchorsIsActive CurrentValue))

(fn GetAnchorsIsActive
  (return (Variables|Default|GetAnchorsIsActive)))

(fn GetAnchorIndex
  (params (ItemToFind :type Sphere%20Component%20Object%20Reference%20%28by%20ref%29))
  (bind _keys (Utilities|Map|Keys (Variables|Default|GetAnchorList)))
  (return (Utilities|Array|FindItem _keys ItemToFind)))

(fn DestroyAllNS
  (bind _ns_anchor (Variables|Default|GetNS_Anchor))
  (for _array_element _ns_anchor
    (Components|DestroyComponent _array_element))
  (Utilities|Array|Clear _ns_anchor)
  (return))

(fn SetRenderActiveNSbyIndex
  (params (Index :type Integer) (IsRendering :type Boolean))
  (bind _ns_anchor (Variables|Default|GetNS_Anchor))
  (bind _output (Utilities|Array|Get(acopy) _ns_anchor Index))
  (LocalVariables|SetCurrentNS _output)
  (if IsRendering
    (LocalVariables|GetCurrentNS
      (:then
        _)
      (:else
        (bind _returnvalue (Niagara|SpawnSystemAttached "/Game/VFX/Niagara/Fish/NS_Anchor.NS_Anchor" _output (Utilities|Array|Get(acopy) (Variables|Default|GetSocketsAnchor) Index) "0, 0, 0" "0, 0, 0" "SnapToTargetIncludingScale" false))
        (LocalVariables|SetCurrentNS _returnvalue)))
    (else
      (bind _currentns (LocalVariables|GetCurrentNS)
        (:then
          (Components|DestroyComponent _currentns))
        (:else
          _))))
  (Utilities|Array|SetArrayElem (Variables|Default|GetNS_Anchor) Index (LocalVariables|GetCurrentNS) true))

(fn SetRenderActiveNSbyAnchor
  (params (Anchor :type Sphere%20Component%20Object%20Reference%20%28by%20ref%29) (IsRendering :type Boolean))
  (Utilities|IsValid Anchor
    (:Is%20Valid
      (CallFunction|SetRenderActiveNSbyIndex (CallFunction|GetAnchorIndex Anchor) IsRendering)
      (return))
    (:Is%20Not%20Valid
      (Development|PrintText "Anchor is not valid to deactive NS"))))