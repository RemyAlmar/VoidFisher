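; Actor component that manages dynamic material instances for the owner's skeletal mesh, found on BeginPlay.
; It creates one instance per key name from a parent material, caches it in a map and applies it to material slot 0.
; Scalar setters look up an instance by key, or by index when the key is empty, and record values in one parameter map shared across all instances.
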(event EventBeginPlay
  (Variables|Default|SetSKM_Owner (Actor|GetComponentbyClass (Components|GetOwner) "/Script/Engine.SkeletalMeshComponent")))

(fn AddNewMaterialInstanceDynamical
  (params (Parent :type Material%20Interface%20Object%20Reference) (KeyName :type String))
  (bind _milist (Variables|Default|GetMIList))
  (if (Utilities|Map|Contains (Variables|Default|GetMIList) KeyName)
    _
    (else
      (bind _returnvalue (Rendering|Material|CreateDynamicMaterialInstance Parent "None" "None" :!class /Script/Engine.KismetMaterialLibrary))
      (Utilities|Map|Add _milist KeyName _returnvalue)))
  (Rendering|Material|SetMaterial (Variables|Default|GetSKM_Owner) 0 (.Value (Utilities|Map|Find _milist KeyName)))
  (return))

(fn GetMIDbyString
  (params (Key :type String))
  (return (.Value (Utilities|Map|Find (Variables|Default|GetMIList) Key))))

(fn GetMIDbyID
  (params (Index :type Integer))
  (if (HandleMIDynamic|HasMatInstDynamic)
    (bind _values (Utilities|Map|Values (Variables|Default|GetMIList)))
    (return (Utilities|Array|Get(acopy) _values Index))))

(fn HasMatInstDynamic
  (return (Utilities|Map|IsNotEmpty (Variables|Default|GetMIList))))

(fn SetScalarParameter
  (params (Key :type String) (Index :type Integer) (ParameterName :type Name) (Value :type Float%20%28single-precision%29))
  (if (Utilities|Enum|Equal(Enum) Key "")
    (LocalVariables|SetLocalMID (HandleMIDynamic|GetMIDbyID Index))
    (else
      (LocalVariables|SetLocalMID (HandleMIDynamic|GetMIDbyString Key))))
  (HandleParameter|AddScalarParameter ParameterName Value)
  (Rendering|Material|SetScalarParameterValue (LocalVariables|GetLocalMID) ParameterName (HandleParameter|GetScalarParameterValue ParameterName) :!class /Script/Engine.MaterialInstanceDynamic)
  (return))

(fn GetScalarParameterValue
  (params (Key :type Name))
  (bind _scalarparameter (Variables|Default|GetScalarParameter))
  (bind (_value _returnvalue) (Utilities|Map|Find _scalarparameter Key))
  (if _returnvalue
    _
    (else
      (HandleParameter|AddScalarParameter Key _value)))
  (LocalVariables|SetParameterValue _value)
  (return (LocalVariables|GetParameterValue)))

(fn AddScalarParameter
  (params (Key :type Name) (Value :type Float%20%28double-precision%29))
  (Utilities|Map|Add (Variables|Default|GetScalarParameter) Key Value)
  (return))

(fn DoesParameterExist
  (params (Key :type Name%20%28by%20ref%29))
  (return (.ReturnValue (Utilities|Map|Find (Variables|Default|GetScalarParameter) Key))))