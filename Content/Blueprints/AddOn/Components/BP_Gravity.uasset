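; Gravity component that pulls physics-simulating components toward its center using two spheres passed in by the owner, an outer atmosphere and an inner ground zone.
; Overlap events move components between an atmosphere list and a center list.
; Tick adds velocity along the pull direction, scaled inversely with distance in the atmosphere and proportionally in the inner zone, without delta time.
; Radii are adjustable and scaled by the owner's largest axis.
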(event Custom|OnBeginOverlapAttracted
  (params (OverlappedComponent :type Primitive%20Component%20Object%20Reference) (OtherActor :type Actor%20Object%20Reference) (OtherComp :type Primitive%20Component%20Object%20Reference) (OtherBodyIndex :type Integer) (bFromSweep :type Boolean) (SweepResult :type Hit%20Result%20Structure%20%28by%20ref%29))
  (Development|PrintString "Begin Overlap")
  (if (Physics|IsSimulatingPhysics OtherComp "None")
    (Utilities|Array|AddUnique (Variables|CustomPhysics|GetListActorAtmosphere) OtherComp)))

(event Custom|OnEndOverlapAttracted
  (params (OverlappedComponent :type Primitive%20Component%20Object%20Reference) (OtherActor :type Actor%20Object%20Reference) (OtherComp :type Primitive%20Component%20Object%20Reference) (OtherBodyIndex :type Integer))
  (Development|PrintString "End Overlap" true true "(R=0.890202,G=0.000000,B=1.000000,A=1.000000)")
  (if (Utilities|Array|ContainsItem (Variables|CustomPhysics|GetListActorAtmosphere) OtherComp)
    (Utilities|Array|RemoveItem (Variables|CustomPhysics|GetListActorAtmosphere) OtherComp)))

(event Custom|OnBeginOverlapStopAttracted
  (params (OverlappedComponent :type Primitive%20Component%20Object%20Reference) (OtherActor :type Actor%20Object%20Reference) (OtherComp :type Primitive%20Component%20Object%20Reference) (OtherBodyIndex :type Integer) (bFromSweep :type Boolean) (SweepResult :type Hit%20Result%20Structure%20%28by%20ref%29))
  (if (Utilities|Array|ContainsItem (Variables|CustomPhysics|GetListActorAtmosphere) OtherComp)
    (Utilities|Array|RemoveItem (Variables|CustomPhysics|GetListActorAtmosphere) OtherComp)
    (Utilities|Array|AddUnique (Variables|CustomPhysics|GetListActorCenter) OtherComp)
    (Development|PrintString "Velocity Remove")))

(event Custom|OnEndOverlapStopAttracted
  (params (OverlappedComponent :type Primitive%20Component%20Object%20Reference) (OtherActor :type Actor%20Object%20Reference) (OtherComp :type Primitive%20Component%20Object%20Reference) (OtherBodyIndex :type Integer))
  (if (Utilities|Array|ContainsItem (Variables|CustomPhysics|GetListActorCenter) OtherComp)
    (Utilities|Array|RemoveItem (Variables|CustomPhysics|GetListActorCenter) OtherComp)
    (Utilities|Array|AddUnique (Variables|CustomPhysics|GetListActorAtmosphere) OtherComp)))

(event EventBeginPlay
  (Collision|BindEventtoOnComponentBeginOverlap (Variables|Default|GetGravityInfluenceArea) (EventDispatchers|CreateEvent :!event Custom|OnBeginOverlapAttracted))
  (Collision|BindEventtoOnComponentEndOverlap (Variables|Default|GetGravityInfluenceArea) (EventDispatchers|CreateEvent :!event Custom|OnEndOverlapAttracted))
  (Collision|BindEventtoOnComponentBeginOverlap (Variables|Default|GetStopGravityInfluenceArea) (EventDispatchers|CreateEvent :!event Custom|OnBeginOverlapStopAttracted))
  (Collision|BindEventtoOnComponentEndOverlap (Variables|Default|GetStopGravityInfluenceArea) (EventDispatchers|CreateEvent :!event Custom|OnEndOverlapStopAttracted)))

(event EventTick
  (params (DeltaSeconds :type Float%20%28single-precision%29))
  (Private|Tick|AttractAllActorsInvertProportionnally (Variables|CustomPhysics|GetListActorAtmosphere) (Variables|Default|GetGravityInfluenceArea) (Variables|Radius|GetStopInfluenceRadius))
  (Private|Tick|AttractAllActorsProportionnally (Variables|CustomPhysics|GetListActorCenter) (Variables|Default|GetStopGravityInfluenceArea) 0.0))

(fn SetInfluenceSphere
  (params (GravityInfluenceArea :type Sphere%20Component%20Object%20Reference) (StopGravityInfluenceArea :type Sphere%20Component%20Object%20Reference))
  (bind _output_get (Variables|Default|SetGravityInfluenceArea GravityInfluenceArea))
  (bind _output_get_2 (Variables|Default|SetStopGravityInfluenceArea StopGravityInfluenceArea))
  (Variables|Radius|SetInfluenceRadius (CallFunction|SetRadiusbyScale (Variables|/Script/Engine.SphereComponent|GetSphereRadius _output_get)))
  (Variables|Radius|SetStopInfluenceRadius (CallFunction|SetRadiusbyScale (Variables|/Script/Engine.SphereComponent|GetSphereRadius _output_get_2))))

(fn ChangeRadiusInfluence
  (params (Target :type Sphere%20Component%20Object%20Reference) (InfluenceRadius :type Float%20%28double-precision%29))
  (if (!= InfluenceRadius 0.0)
    (Components|Sphere|SetSphereRadius Target InfluenceRadius true)))

(fn AttractAllActorsInvertProportionnally
  (params (Array :type Array%20of%20Primitive%20Component%20Object%20References) (InfluenceArea :type Scene%20Component%20Object%20Reference) (LimitRadiusInfluence :type Float%20%28double-precision%29))
  (if (Utilities|Array|IsNotEmpty Array)
    (for _array_element Array
      (Utilities|IsValid (Components|GetOwner _array_element)
        (:Is%20Valid
          (bind _output_get (LocalVariables|SetAttractedDirection (Math|Vector|Normalize (- (Transformation|GetWorldLocation InfluenceArea) (Transformation|GetWorldLocation _array_element)))))
          (Development|PrintString (Utilities|String|ToString(Float) (* (Variables|Gravity|GetAtmosphereGravityForce) (/ (CallFunction|GetDistanceMax (Variables|Radius|GetInfluenceRadius) LimitRadiusInfluence) (Math|Vector|Distance(Vector) (CallFunction|GetPointfromCenter (LocalVariables|GetAttractedDirection) LimitRadiusInfluence) (Transformation|GetWorldLocation _array_element))))) true true "(R=0.819650,G=1.000000,B=0.000000,A=1.000000)" 0.0)
          (Physics|SetPhysicsLinearVelocity _array_element (* _output_get (* (Variables|Gravity|GetAtmosphereGravityForce) (/ (CallFunction|GetDistanceMax (Variables|Radius|GetInfluenceRadius) LimitRadiusInfluence) (Math|Vector|Distance(Vector) (CallFunction|GetPointfromCenter (LocalVariables|GetAttractedDirection) LimitRadiusInfluence) (Transformation|GetWorldLocation _array_element))))) true "None"))))
    (return)))

(fn SetRadiusbyScale
  (params (OriginRadius :type Float%20%28double-precision%29))
  (bind _returnvalue (Components|GetOwner))
  (bind _returnvalue_2 (Transformation|GetActorScale3D _returnvalue))
  (return (* OriginRadius (Math|Float|Max(Float) (Math|Float|Max(Float) (.x _returnvalue_2) (.y _returnvalue_2)) (.z _returnvalue_2)))))

(fn GetPointfromCenter
  (params (NormalizeDirection :type Vector) (Length :type Float%20%28double-precision%29))
  (return (+ (Transformation|GetActorLocation (Components|GetOwner)) (* NormalizeDirection Length))))

(fn GetDistanceMax
  (params (StartInfluence :type Float%20%28double-precision%29) (EndInfluence :type Float%20%28double-precision%29))
  (return (- StartInfluence EndInfluence)))

(fn AttractAllActorsProportionnally
  (params (Array :type Array%20of%20Primitive%20Component%20Object%20References) (InfluenceArea :type Scene%20Component%20Object%20Reference) (LimitRadiusInfluence :type Float%20%28double-precision%29))
  (if (Utilities|Array|IsNotEmpty Array)
    (for _array_element Array
      (Utilities|IsValid (Components|GetOwner _array_element)
        (:Is%20Valid
          (bind _output_get (LocalVariables|SetAttractedDirection (Math|Vector|Normalize (- (Transformation|GetWorldLocation InfluenceArea) (Transformation|GetWorldLocation _array_element)))))
          (Development|PrintString (Utilities|String|ToString(Float) (* (Variables|Gravity|GetGroundGravityForce) (/ (Math|Vector|Distance(Vector) (CallFunction|GetPointfromCenter (LocalVariables|GetAttractedDirection) LimitRadiusInfluence) (Transformation|GetWorldLocation _array_element)) (CallFunction|GetDistanceMax (Variables|Radius|GetStopInfluenceRadius) LimitRadiusInfluence)))) true true "(R=0.819650,G=1.000000,B=0.000000,A=1.000000)" 0.0)
          (Physics|SetPhysicsLinearVelocity _array_element (* _output_get (* (Variables|Gravity|GetGroundGravityForce) (/ (Math|Vector|Distance(Vector) (CallFunction|GetPointfromCenter (LocalVariables|GetAttractedDirection) LimitRadiusInfluence) (Transformation|GetWorldLocation _array_element)) (CallFunction|GetDistanceMax (Variables|Radius|GetStopInfluenceRadius) LimitRadiusInfluence)))) true "None"))))
    (return)))

(fn ChangeAtmosphereRadius
  (params (InfluenceRadius :type Float%20%28double-precision%29))
  (bind _gravityinfluencearea (Variables|Default|GetGravityInfluenceArea))
  (Private|Radius|ChangeRadiusInfluence _gravityinfluencearea InfluenceRadius)
  (Variables|Radius|SetInfluenceRadius (CallFunction|SetRadiusbyScale (Variables|/Script/Engine.SphereComponent|GetSphereRadius _gravityinfluencearea))))

(fn ChangeGroundRadius
  (params (Radius :type Float%20%28double-precision%29))
  (bind _stopgravityinfluencearea (Variables|Default|GetStopGravityInfluenceArea))
  (Private|Radius|ChangeRadiusInfluence _stopgravityinfluencearea Radius)
  (Variables|Radius|SetStopInfluenceRadius (CallFunction|SetRadiusbyScale (Variables|/Script/Engine.SphereComponent|GetSphereRadius _stopgravityinfluencearea))))