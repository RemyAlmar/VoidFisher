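; BPC_BounceManager is an actor component that makes its owner bounce off impacts, working through the sibling BPC_ActorPhysicsMovement component.
; Root hits facing against forward nudge target direction, change speed and set bounce power from pre-impact speed.
; Fast enough hits, unless invulnerable, start temporary invulnerability, fire a hit event and time a bounce by speed and impact angle.
; Tick applies bounce force and steering scaled by remaining time, and ends invulnerability.
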(event Custom|Root_OnComponentHit
  (params (HitComponent :type Primitive%20Component%20Object%20Reference) (OtherActor :type Actor%20Object%20Reference) (OtherComp :type Primitive%20Component%20Object%20Reference) (NormalImpulse :type Vector) (Hit :type Hit%20Result%20Structure%20%28by%20ref%29))
  (bind (_bblockinghit _binitialoverlap _time _distance _location _impactpoint _normal _impactnormal) (Collision|BreakHitResult Hit))
  (bind _impactnormal_2 (Collision|BreakHitResult Hit))
  (bind _bpc_actorphysics (Variables|Default|GetBPC_ActorPhysics))
  (if (CallFunction|CanBounce _impactnormal_2)
    (Variables|/Game/Blueprints/AddOn/Components/BPC_ActorPhysicsMovement.BPC_ActorPhysicsMovement_C|SetTargetDirection _bpc_actorphysics (+ (Variables|/Game/Blueprints/AddOn/Components/BPC_ActorPhysicsMovement.BPC_ActorPhysicsMovement_C|GetTargetDirection _bpc_actorphysics) (* _impactnormal_2 1e+01)))
    (bind _previousspeedvalue (CallFunction|Bounced (Math|Vector|VectorLength (Variables|/Game/Blueprints/AddOn/Components/BPC_ActorPhysicsMovement.BPC_ActorPhysicsMovement_C|GetSelfForce (Variables|Default|GetBPC_ActorPhysics))) _impactnormal_2))
    (if (>= _previousspeedvalue (CallFunction|GetMinSpeedtoBounce))
      (if (not (Variables|Invulnerability|GetIsInvulnerable))
        (bind _output_get (Variables|Bounce|SetBounceTimeMax (CallFunction|CalculBounceTimeMax _previousspeedvalue _impactnormal_2)))
        (Variables|Bounce|SetBounceTime _output_get)
        (Variables|Invulnerability|SetIsInvulnerable true)
        (Default|CallEDonHit _impactpoint (Math|Rotator|MakeRotfromZ _impactnormal))))))

(event EventTick
  (params (DeltaSeconds :type Float%20%28single-precision%29))
  (bind _bouncepower (Variables|Bounce|GetBouncePower))
  (bind _bouncetime (Variables|Bounce|GetBounceTime))
  (bind _bpc_actorphysics (Variables|Default|GetBPC_ActorPhysics))
  (bind _returnvalue (* _bouncepower _bouncetime))
  (Utilities|FlowControl|Sequence
    (:then_0
      (if (Variables|Invulnerability|GetIsInvulnerable)
        (if (CallFunction|TimerPos (Variables|Invulnerability|Time|GetCurrentTime_Invulnerability) (Variables|Invulnerability|Time|GetMaxTime_Invulnerability) 1.0 true)
          (Variables|Invulnerability|SetIsInvulnerable false)
          (Default|CallEDonStopInvulnerability))))
    (:then_1
      (if (!= (Variables|Bounce|GetBounceTime) 0.0)
        (if (not (CallFunction|TimerNeg (Variables|Bounce|GetBounceTime) (Variables|Bounce|GetBounceTimeMax) 1.0 false))
          (Default|SetOtherForcesMovement _bpc_actorphysics _returnvalue)
          (Variables|/Game/Blueprints/AddOn/Components/BPC_ActorPhysicsMovement.BPC_ActorPhysicsMovement_C|SetTargetDirection _bpc_actorphysics (+ (Variables|/Game/Blueprints/AddOn/Components/BPC_ActorPhysicsMovement.BPC_ActorPhysicsMovement_C|GetTargetDirection _bpc_actorphysics) (* (Math|Vector|Normalize _returnvalue) _bouncetime))))))))

(event EventBeginPlay
  (bind _returnvalue (Components|GetOwner))
  (bind _returnvalue_2 (Actor|GetComponentbyClass _returnvalue "/Game/Blueprints/AddOn/Components/BPC_ActorPhysicsMovement.BPC_ActorPhysicsMovement_C"))
  (Utilities|IsValid _returnvalue_2
    (:Is%20Valid
      (bind _output_get (Variables|Default|SetBPC_ActorPhysics _returnvalue_2))
      (Collision|BindEventtoOnComponentHit (Variables|/Game/Blueprints/AddOn/Components/BPC_ActorPhysicsMovement.BPC_ActorPhysicsMovement_C|GetOwnRootPhysics _output_get) (EventDispatchers|CreateEvent :!event Custom|Root_OnComponentHit)))))

(fn Bounced
  (params (Speed :type Float%20%28double-precision%29) (ImpactNormal :type Vector))
  (bind _bpc_actorphysics (Variables|Default|GetBPC_ActorPhysics))
  (LocalVariables|SetPreviousSpeed Speed)
  (Default|ChangeSpeedonImpact _bpc_actorphysics ImpactNormal)
  (Variables|Bounce|SetBouncePower (* (Default|GetBoundDirection _bpc_actorphysics ImpactNormal) (LocalVariables|GetPreviousSpeed)))
  (return (LocalVariables|GetPreviousSpeed)))

(fn CalculBounceTimeMax
  (params (CurrentSpeed :type Float%20%28double-precision%29) (ImpactNormal :type Vector))
  ;[1 0.3831 0] Recupere un float basé sur le DOT entre l'impact et le forward ainsi que sur la vitesse d'impact normalisé par rapport à la vitesse max mulitplié par un multiplicateur de temps
  (return (* (Math|Float|NormalizetoRange CurrentSpeed 0.0 (Variables|Speed|GetMaxSpeed)) (* (Math|Float|Absolute(Float) (Math|Vector|DotProduct ImpactNormal (Math|Vector|GetForwardVector (Variables|/Game/Blueprints/AddOn/Components/BPC_ActorPhysicsMovement.BPC_ActorPhysicsMovement_C|GetOwnRootPhysics (Variables|Default|GetBPC_ActorPhysics))))) (Variables|Speed|GetLoseControlTimeMax)))))

(fn GetSpeedMaxPercent
  (return (* (/ (Variables|Speed|GetMaxSpeed) 1e+02) (Variables|Speed|GetPercentMaxSpeedToApplyImpact))))

(fn CanBounce
  (params (ImpactNormal :type Vector))
  (return (<= (Math|Vector|DotProduct ImpactNormal (Math|Vector|GetForwardVector (Variables|/Game/Blueprints/AddOn/Components/BPC_ActorPhysicsMovement.BPC_ActorPhysicsMovement_C|GetOwnRootPhysics (Variables|Default|GetBPC_ActorPhysics)))) (Variables|Bounce|GetAngleMinToImpact))))

(fn GetMinSpeedtoBounce
  (return (Math|Float|Min(Float) (Variables|Speed|GetMinSpeedToApplyImpact) (CallFunction|GetSpeedMaxPercent))))