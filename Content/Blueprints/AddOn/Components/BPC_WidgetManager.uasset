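; BPC_WidgetManager is a component that manages screen widgets and 3D world widgets attached to actors.
; Screen widgets are created conditionally from a given class, added to the viewport and accompanied by a 2D sound.
; World widgets spawn as BP_WorldWidget actors at the parent's transform, attach to it and are tracked in ListWorldWidget.
; Removal by reference or list index takes the actor off that list and destroys it.
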(fn AddWidgettoPlayerScreen
  (params (Target :type User%20Widget%20Class%20Reference) (Condition :type Boolean))
  (if Condition
    (bind _returnvalue (UserInterface|CreateWidget Target))
    (UserInterface|Viewport|AddtoViewport _returnvalue 10)
    (Audio|PlaySound2D "/Game/SFX/Sounds/NEW_OGG/Creatures/SFX_Attaque_Shineon_1_Cue.SFX_Attaque_Shineon_1_Cue" 1.0 1.0 0.0 0 0)))

(fn AddWidget3DtoActor
  (params (WidgetToSpawn :type Widget%20Component%20Object%20Reference) (ParentActor :type Actor%20Object%20Reference))
  (bind _returnvalue (Game|SpawnActorfromClass "/Game/Blueprints/Game/Miscellanious/BP_WorldWidget.BP_WorldWidget_C" (Transformation|GetActorTransform ParentActor) "Undefined" "MultiplyWithRoot" 0 WidgetToSpawn 0))
  (LocalVariables|SetCurrentWidget _returnvalue)
  (Transformation|AttachActorToActor (LocalVariables|GetCurrentWidget) ParentActor "None" "KeepWorld" "KeepWorld" "KeepWorld" true)
  (Utilities|Array|Add (Variables|Default|GetListWorldWidget) (LocalVariables|GetCurrentWidget))
  (return))

(fn Remove3DWidget
  (params (Item :type BP%20World%20Widget%20Object%20Reference%20%28by%20ref%29))
  (LocalVariables|SetWidgetToDestroy Item)
  (Utilities|Array|RemoveItem (Variables|Default|GetListWorldWidget) (LocalVariables|GetWidgetToDestroy))
  (Actor|DestroyActor (LocalVariables|GetWidgetToDestroy))
  (return))

(fn Remove3DWidgetbyIndex
  (params (Index :type Integer))
  (bind _output_get (LocalVariables|SetWidgetToDestroy (Utilities|Array|Get(acopy) (Variables|Default|GetListWorldWidget) Index)))
  (CallFunction|Remove3DWidget _output_get)
  (return))