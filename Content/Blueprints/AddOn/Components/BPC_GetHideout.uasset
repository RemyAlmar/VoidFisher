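; Actor component that lets its owner find and hide inside BP_Hideout actors.
; A supplied sphere collider records hideouts it overlaps, and queries pick the nearest known one, favoring unfilled ones, for location or direction.
; Enter and leave events track the current hideout, toward which PlaceSelfInHideout interpolates the owner with sweep.
; On arrival it notifies the hideout; enter, leave and reach are relayed through event dispatchers.
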(event Custom|SphereColl_OnComponentBeginOverlap_Event
  (params (OverlappedComponent :type Primitive%20Component%20Object%20Reference) (OtherActor :type Actor%20Object%20Reference) (OtherComp :type Primitive%20Component%20Object%20Reference) (OtherBodyIndex :type Integer) (bFromSweep :type Boolean) (SweepResult :type Hit%20Result%20Structure%20%28by%20ref%29))
  (bind _asbp_hideout (Utilities|Casting|CastToBP_Hideout OtherActor))
  (CallFunction|AddHideoutKnown _asbp_hideout))

(event Custom|OnHideoutReached
  (params (Target :type BP%20Hideout%20Object%20Reference))
  (Utilities|IsValid Target
    (:Is%20Valid
      (Default|OnActorHiddeninHideout Target (Components|GetOwner))
      (Default|CallEDonHideoutReached Target))))

(event Custom|OnHideoutEnter
  (params (Target :type BP%20Hideout%20Object%20Reference))
  (bind _output_get (Variables|Default|SetCurrentHideout Target))
  (Default|CallEDonHideoutEnter _output_get))

(event Custom|OnHideoutLeaved
  (params (Target :type BP%20Hideout%20Object%20Reference))
  (Variables|Default|SetCurrentHideout 0)
  (Default|CallEDonHideoutLeaved Target))

(fn Initialize
  (params (SphereCollider :type Sphere%20Component%20Object%20Reference))
  (bind _output_get (Variables|Default|SetSphereCollider SphereCollider))
  (Collision|BindEventtoOnComponentBeginOverlap _output_get (EventDispatchers|CreateEvent :!event Custom|SphereColl_OnComponentBeginOverlap_Event)))

(fn GetNearestHideout
  (bind _hideouts (Variables|Default|GetHideouts))
  (if (CallFunction|HasHideoutKnown)
    (bind _output_get (LocalVariables|SetHideoutNearest (Utilities|Array|Get(acopy) _hideouts (Utilities|Array|LastIndex _hideouts))))
    (LocalVariables|SetDistanceMax (CallFunction|GetDistancewithHideout _output_get))
    (for _array_element (Variables|Default|GetHideouts)
      (if (Variables|/Game/Blueprints/Game/Environment/BP_Hideout.BP_Hideout_C|GetIsFilled _array_element)
        (if (== (LocalVariables|GetHideoutNearest) (LocalVariables|GetLCurrentHideout))
          (LocalVariables|SetHideoutNearest 0))
        (else
          (bind _output_get_2 (LocalVariables|SetLCurrentHideout _array_element))
          (LocalVariables|SetCurrentDistance (CallFunction|GetDistancewithHideout _output_get_2))
          (if (< (LocalVariables|GetCurrentDistance) (LocalVariables|GetDistanceMax))
            (LocalVariables|SetHideoutNearest (LocalVariables|GetLCurrentHideout) :!label _label)
            (LocalVariables|SetDistanceMax (LocalVariables|GetCurrentDistance))
            (else
              (bind _hideoutnearest (LocalVariables|GetHideoutNearest)
                (:then
                  (if (Variables|/Game/Blueprints/Game/Environment/BP_Hideout.BP_Hideout_C|GetIsFilled _hideoutnearest)
                    (goto _label)))
                (:else
                  (goto _label))))))))
    (return (LocalVariables|GetHideoutNearest))))

(fn GetDistancewithHideout
  (params (TargetHideout :type Actor%20Object%20Reference))
  (Utilities|IsValid TargetHideout
    (:Is%20Valid
      (LocalVariables|SetDistance (Math|Vector|Distance(Vector) (Transformation|GetActorLocation TargetHideout) (Transformation|GetActorLocation (Components|GetOwner)))))
    (:Is%20Not%20Valid
      _))
  (return (LocalVariables|GetDistance)))

(fn HasHideoutKnown
  (return (Utilities|Array|IsNotEmpty (Variables|Default|GetHideouts))))

(fn GetNearestHideoutLocation
  (LocalVariables|SetNearestHideout (CallFunction|GetNearestHideout))
  (Utilities|IsValid (LocalVariables|GetNearestHideout)
    (:Is%20Valid
      (bind _output_get (LocalVariables|SetpIsValid (not (Variables|/Game/Blueprints/Game/Environment/BP_Hideout.BP_Hideout_C|GetIsFilled (LocalVariables|GetNearestHideout)))))
      (if _output_get
        (LocalVariables|SetCurrActorLocation (Transformation|GetActorLocation (LocalVariables|GetNearestHideout)))))
    (:Is%20Not%20Valid
      _))
  (return (LocalVariables|GetpIsValid) (LocalVariables|GetCurrActorLocation)))

(fn GetNearestHideoutDirection
  (bind (_isvalid _returnvalue) (CallFunction|GetNearestHideoutLocation))
  (LocalVariables|SetDirection _returnvalue)
  (LocalVariables|SetlIsValid _isvalid)
  (LocalVariables|SetDirection (Math|Vector|GetUnitDirection(Vector) (Transformation|GetActorLocation (Components|GetOwner)) (LocalVariables|GetDirection)))
  (return (LocalVariables|GetlIsValid) (LocalVariables|GetDirection)))

(fn AddHideoutKnown
  (params (Target :type BP%20Hideout%20Object%20Reference))
  (bind _hideouts (Variables|Default|GetHideouts))
  (if (Utilities|Array|ContainsItem _hideouts Target)
    _
    (else
      (Utilities|Array|AddUnique _hideouts Target)))
  (return))

(fn SetWanttoHideSelf
  (params (WantToHideSelf :type Boolean))
  (LocalVariables|SetPreviousValue (Variables|Default|GetWantToHideSelf))
  (Variables|Default|SetWantToHideSelf WantToHideSelf)
  (if (!= (Variables|Default|GetWantToHideSelf) (LocalVariables|GetPreviousValue))
    _))

(fn PlaceSelfinHideout
  (params (InterpSpeed :type Float%20%28single-precision%29))
  (bind _returnvalue (Components|GetOwner))
  (bind _returnvalue_2 (Transformation|GetActorLocation _returnvalue))
  (bind _currenthideout (Variables|Default|GetCurrentHideout)
    (:then
      (Transformation|SetActorLocation _returnvalue (Math|Interpolation|VInterpTo _returnvalue_2 (Transformation|GetActorLocation _currenthideout) (Utilities|Time|GetWorldDeltaSeconds) InterpSpeed) true false)
      (CallFunction|SetHidden (Utilities|Operators|EqualEqual _returnvalue_2 (Transformation|GetActorLocation _currenthideout) 0.0))
      (return))
    (:else)))

(fn SetHidden
  (params (IsHidden :type Boolean))
  (LocalVariables|SetPreviousValue (Variables|Default|GetIsHidden))
  (Variables|Default|SetIsHidden IsHidden)
  (if (!= (Variables|Default|GetIsHidden) (LocalVariables|GetPreviousValue))
    (if (Variables|Default|GetIsHidden)
      (CallFunction|OnHideoutReached (Variables|Default|GetCurrentHideout)))))