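; Shared function library of gameplay helpers for timers, value ramps, vector math, physics, randomization, timecode differences and Niagara socket spawning.
; By-ref timers advance with world delta time and drive the timed increase and decrease functions.
; Direction finders fire rings of line traces in widening cones and pick a random unblocked ray, such as for obstacle avoidance.
; Other helpers launch or stop physics actors, align rotations with quaternion slerp and set constraint limits.
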(fn GetSignedValue
  (params (Value :type Float%20%28double-precision%29))
  (return (/ Value (Math|Float|Absolute(Float) Value))))

(fn TimerPos
  (params (CurrentTime :type Float%20%28double-precision%29%20%28by%20ref%29) (MaxTime :type Float%20%28double-precision%29) (DeltaTimeMultiplier :type Float%20%28double-precision%29) (AutoResetTimer :type Boolean))
  (bind _output_get (LocalVariables|SetFutureTime (+ CurrentTime (* (Utilities|Time|GetWorldDeltaSeconds) DeltaTimeMultiplier))))
  (bind _output_get_2 (LocalVariables|SetTimeReached (>= _output_get MaxTime)))
  (if _output_get_2
    (if AutoResetTimer
      (LocalVariables|SetFutureTime 0.0)
      (else
        (LocalVariables|SetFutureTime MaxTime))))
  (|SetBy-RefVar CurrentTime (LocalVariables|GetFutureTime))
  (return (LocalVariables|GetTimeReached)))

(fn TimerNeg
  (params (CurrentTime :type Float%20%28double-precision%29%20%28by%20ref%29) (TimeMax :type Float%20%28double-precision%29) (DeltaTimeMultiplier :type Float%20%28double-precision%29) (AutoResetTimer :type Boolean))
  (LocalVariables|SetFutureTime (- CurrentTime (* (Utilities|Time|GetWorldDeltaSeconds) DeltaTimeMultiplier)))
  (bind _output_get (LocalVariables|SetTimeSpended (<= (LocalVariables|GetFutureTime) 0.0)))
  (if _output_get
    (if AutoResetTimer
      (LocalVariables|SetFutureTime TimeMax)
      (else
        (LocalVariables|SetFutureTime 0.0))))
  (|SetBy-RefVar CurrentTime (LocalVariables|GetFutureTime))
  (return (LocalVariables|GetTimeSpended)))

(fn IncreaseValueinTime
  (params (ValueToIncrease :type Float%20%28double-precision%29%20%28by%20ref%29) (CurrentTime :type Float%20%28double-precision%29%20%28by%20ref%29) (DeltaTimeMultiplier :type Float%20%28double-precision%29) (ValueMax :type Float%20%28double-precision%29) (TimeMax :type Float%20%28double-precision%29) (AutoResetTimer :type Boolean))
  (if (Timer|TimerPos CurrentTime TimeMax DeltaTimeMultiplier AutoResetTimer)
    (|SetBy-RefVar ValueToIncrease ValueMax)
    (else
      (|SetBy-RefVar ValueToIncrease (* ValueMax (Math|Float|NormalizetoRange (Math|Float|Lerp 0.0 TimeMax (/ CurrentTime TimeMax)) 0.0 TimeMax)))))
  (|SetBy-RefVar ValueToIncrease (Math|Float|Clamp(Float) ValueToIncrease 0.0 ValueMax))
  (return ValueToIncrease))

(fn DecreaseValueinTime
  (params (ValueToDecreased :type Float%20%28double-precision%29%20%28by%20ref%29) (CurrentTime :type Float%20%28double-precision%29%20%28by%20ref%29) (DeltaTime :type Float%20%28double-precision%29) (SpeedMutliplierToDecrease :type Float%20%28double-precision%29) (TimeMax :type Float%20%28double-precision%29) (ValueMax :type Float%20%28double-precision%29) (AutoResetTimer :type Boolean))
  (if (Timer|TimerNeg CurrentTime TimeMax SpeedMutliplierToDecrease AutoResetTimer)
    _
    (else
      _))
  (|SetBy-RefVar ValueToDecreased (* ValueMax (Math|Float|NormalizetoRange (Math|Float|Lerp 0.0 TimeMax (/ CurrentTime TimeMax)) 0.0 TimeMax)))
  (|SetBy-RefVar ValueToDecreased (Math|Float|Clamp(Float) ValueToDecreased 0.0 ValueMax))
  (return ValueToDecreased))

(fn IncreaseValueExp
  (params (ValueToIncrease :type Float%20%28double-precision%29%20%28by%20ref%29) (InputValue :type Float%20%28double-precision%29) (ValueToAdd :type Float%20%28double-precision%29) (Exp :type Float%20%28double-precision%29) (ClampValueMax :type Float%20%28double-precision%29))
  (|SetBy-RefVar ValueToIncrease (Math|Float|Clamp(Float) (+ ValueToIncrease (* InputValue (Math|Float|Power ValueToAdd Exp))) 0.0 ClampValueMax))
  (return))

(fn DecreaseValueExp
  (params (ValueToDecrease :type Float%20%28double-precision%29%20%28by%20ref%29) (InputValue :type Float%20%28double-precision%29) (ValueToSubstract :type Float%20%28double-precision%29) (Exp :type Float%20%28double-precision%29) (ClampValueMax :type Float%20%28double-precision%29))
  (|SetBy-RefVar ValueToDecrease (Math|Float|Clamp(Float) (- ValueToDecrease (* InputValue (Math|Float|Power ValueToSubstract Exp))) 0.0 ClampValueMax))
  (return))

(fn LaunchActor
  (params (ActorToLaunch :type Actor%20Object%20Reference) (Direction :type Vector) (LaunchPower :type Float%20%28double-precision%29) (ParentVelocity :type Vector))
  (Utilities|IsValid ActorToLaunch
    (:Is%20Valid
      (bind _asprimitive_component (Utilities|Casting|CastToPrimitiveComponent (Variables|/Script/Engine.Actor|GetRootComponent ActorToLaunch)))
      (bind _output_get (LocalVariables|SetPrimitiveRoot _asprimitive_component))
      (if (Physics|IsSimulatingPhysics _output_get "None")
        _
        (else
          (Physics|SetSimulatePhysics _output_get true)))
      (Physics|SetPhysicsLinearVelocity _output_get (* (+ (Math|Vector|VectorLength ParentVelocity) LaunchPower) Direction) false "None"))))

(fn PointForwardActor
  (params (Target :type Actor%20Object%20Reference) (Distance :type Float%20%28single-precision%29))
  (return (+ (Transformation|GetActorLocation Target) (* (Transformation|GetActorForwardVector Target) Distance))))

(fn ConeTracebyChannel
  (params (RaysNumber :type Integer) (Origin :type Vector) (Direction :type Vector) (ConeAngle :type Float%20%28double-precision%29) (Range :type Float%20%28double-precision%29))
  (LocalVariables|SetHalfAngle (/ ConeAngle 2.0))
  (LocalVariables|SetRightVector (Math|Vector|Normalize (Math|Vector|CrossProduct (Math|Vector|VectorUp) Direction)))
  (LocalVariables|SetUpVector (Math|Vector|Normalize (Math|Vector|CrossProduct Direction (LocalVariables|GetRightVector))))
  (for _index (range 1 RaysNumber)
    (LocalVariables|SetAngleAroundAxis (/ (* 360 (- _index 1)) RaysNumber))
    (LocalVariables|SetEdgeDirection (Math|Vector|RotateVectorAroundAxis Direction (LocalVariables|GetHalfAngle) (LocalVariables|GetRightVector)))
    (bind _output_get (LocalVariables|SetRayDirection (Math|Vector|RotateVectorAroundAxis (LocalVariables|GetEdgeDirection) (LocalVariables|GetAngleAroundAxis) Direction)))
    (bind (_outhit _returnvalue) (Collision|LineTraceByChannel 0 Origin (+ Origin (* _output_get Range)) "TraceTypeQuery1" false 0 "ForOneFrame" true "(R=1.000000,G=0.000000,B=0.000000,A=1.000000)" "(R=0.000000,G=1.000000,B=0.000000,A=1.000000)" 0.0))
    (Utilities|Array|Add (LocalVariables|GetOutHits) _outhit)
    (Utilities|Array|Add (LocalVariables|GetHits) _returnvalue))
  (return (LocalVariables|GetOutHits) (LocalVariables|GetHits)))

(fn ConeTracebyChannelNotHit
  (params (RaysNumber :type Integer) (Origin :type Vector) (Direction :type Vector) (ConeAngle :type Float%20%28double-precision%29) (Range :type Float%20%28double-precision%29) (TraceChannel :type ETraceTypeQuery%20Enum :default "TraceTypeQuery1") (DrawDebugType :type EDrawDebugTrace%20Enum :default "None") (DrawTime :type Float%20%28single-precision%29) (TraceColor :type Linear%20Color%20Structure))
  (bind _raydirectionout (LocalVariables|GetRayDirectionOut))
  (LocalVariables|SetHalfAngle (/ ConeAngle 2.0))
  (LocalVariables|SetRightVector (Math|Vector|Normalize (Math|Vector|CrossProduct (Math|Vector|VectorUp) Direction)))
  (LocalVariables|SetUpVector (Math|Vector|Normalize (Math|Vector|CrossProduct Direction (LocalVariables|GetRightVector))))
  (for _index (range 1 RaysNumber)
    (LocalVariables|SetAngleAroundAxis (/ (* 360 (- _index 1)) RaysNumber))
    (LocalVariables|SetEdgeDirection (Math|Vector|RotateVectorAroundAxis Direction (LocalVariables|GetHalfAngle) (LocalVariables|GetRightVector)))
    (bind _output_get (LocalVariables|SetRayDirection (Math|Vector|RotateVectorAroundAxis (LocalVariables|GetEdgeDirection) (LocalVariables|GetAngleAroundAxis) Direction)))
    (bind _returnvalue (Collision|LineTraceByChannel 0 Origin (+ Origin (* _output_get Range)) TraceChannel false 0 DrawDebugType true TraceColor "(R=0.000000,G=1.000000,B=0.000000,A=1.000000)" DrawTime))
    (if (not _returnvalue)
      (Utilities|Array|Add (LocalVariables|GetRayDirectionOut) (LocalVariables|GetRayDirection))))
  (return _raydirectionout (Utilities|Array|IsEmpty _raydirectionout)))

(fn GetOneDirectionfromSphereRadius
  (params (RaysNumber :type Integer) (Origin :type Vector) (Direction :type Vector) (ConeAngle :type Float%20%28double-precision%29) (Range :type Float%20%28double-precision%29) (RadiusToCover :type Integer) (TraceChannel :type ETraceTypeQuery%20Enum :default "TraceTypeQuery1") (DrawDebugType :type EDrawDebugTrace%20Enum :default "None") (DrawTime :type Float%20%28single-precision%29) (TraceColor :type Linear%20Color%20Structure) (ActorsToIgnore :type Array%20of%20Actor%20Object%20References))
  (LocalVariables|SetHalfAngle (/ ConeAngle 2.0))
  (LocalVariables|SetRightVector (Math|Vector|Normalize (Math|Vector|CrossProduct (Math|Vector|VectorUp) Direction)))
  (for _index (range 1 (/ RadiusToCover ConeAngle))
    (bind (_raydirectionoutvalue _allhit) (Raycast|ConeTracebyChannelNotHitImproved RaysNumber Origin Direction (Math|Conversions|ToFloat(Integer) (* _index (LocalVariables|GetHalfAngle))) Range TraceChannel DrawDebugType DrawTime TraceColor (LocalVariables|GetRightVector) ActorsToIgnore))
    (LocalVariables|SetDirectionsToGo _raydirectionoutvalue)
    (if (not _allhit) ; If no direction is viable
      (bind _output_get (LocalVariables|SetHasADirectionViable true))
      (if (and _output_get (<= RadiusToCover (* _index (LocalVariables|GetHalfAngle))))
        (LocalVariables|SetDirectionToGo (Utilities|Array|Get(acopy) (LocalVariables|GetDirectionsToGo) (Math|Random|RandomInteger (Utilities|Array|LastIndex (LocalVariables|GetDirectionsToGo)))))
        (if (Class|KismetMathLibrary|EqualExactlyVectorVector (LocalVariables|GetDirectionToGo) "0, 0, 0")
          (LocalVariables|SetDirectionToGo (Math|Random|RandomUnitVectorinConeinDegrees Direction 9e+01)))
        (return (LocalVariables|GetDirectionToGo) (LocalVariables|GetHasADirectionViable)))))
  (if (Class|KismetMathLibrary|EqualExactlyVectorVector (LocalVariables|GetDirectionToGo) "0, 0, 0")
    (LocalVariables|SetDirectionToGo (Math|Random|RandomUnitVectorinConeinDegrees Direction 9e+01)))
  (return (LocalVariables|GetDirectionToGo) (LocalVariables|GetHasADirectionViable)))

(fn AlignVectors
  (params (ActorRotation :type Scene%20Component%20Object%20Reference) (Goal :type Vector))
  (bind _output_get (LocalVariables|SetCurrentRotationQuat (Math|Conversions|ToQuaternion(Rotator) (Variables|/Script/Engine.SceneComponent|GetRelativeRotation ActorRotation))))
  (bind _output_get_2 (LocalVariables|SetTargetRotationQuat (* (Class|KismetMathLibrary|QuatFindBetweenNormals (Math|Vector|GetForwardVector ActorRotation) (Math|Vector|Normalize Goal)) _output_get)))
  (return (LocalVariables|GetCurrentRotationQuat) _output_get_2))

(fn AlignSmooth
  (params (CurrentRota :type Quat%20Structure%20%28by%20ref%29) (TargetRota :type Quat%20Structure%20%28by%20ref%29) (InterpolationSpeed :type Float%20%28double-precision%29))
  (LocalVariables|SetPassRotation (Class|KismetMathLibrary|QuatSlerp CurrentRota TargetRota (* InterpolationSpeed (Utilities|Time|GetWorldDeltaSeconds))))
  (return (Class|KismetMathLibrary|QuatRotator (LocalVariables|GetPassRotation))))

(fn ConeTracebyChannelNotHitImproved
  (params (RaysNumber :type Integer) (Origin :type Vector) (Direction :type Vector) (HalfAngle :type Float%20%28double-precision%29) (Range :type Float%20%28double-precision%29) (TraceChannel :type ETraceTypeQuery%20Enum :default "TraceTypeQuery1") (DrawDebugType :type EDrawDebugTrace%20Enum :default "None") (DrawTime :type Float%20%28single-precision%29) (TraceColor :type Linear%20Color%20Structure) (RightVector :type Vector) (ActorsToIgnore :type Array%20of%20Actor%20Object%20References))
  (bind _raydirectionout (LocalVariables|GetRayDirectionOut))
  (for _index (range 1 RaysNumber)
    (LocalVariables|SetAngleAroundAxis (/ (* 360 (- _index 1)) RaysNumber))
    (LocalVariables|SetEdgeDirection (Math|Vector|RotateVectorAroundAxis Direction HalfAngle RightVector))
    (bind _output_get (LocalVariables|SetRayDirection (Math|Vector|RotateVectorAroundAxis (LocalVariables|GetEdgeDirection) (LocalVariables|GetAngleAroundAxis) Direction)))
    (bind _returnvalue (Collision|LineTraceByChannel 0 Origin (+ Origin (* _output_get Range)) TraceChannel false ActorsToIgnore DrawDebugType true TraceColor "(R=1.000000,G=0.055641,B=0.000000,A=1.000000)" DrawTime))
    (if (not _returnvalue)
      (Utilities|Array|Add (LocalVariables|GetRayDirectionOut) (LocalVariables|GetRayDirection))))
  (return _raydirectionout (Utilities|Array|IsEmpty _raydirectionout)))

(fn GetOneDirectionfromFirstConeNoHit
  (params (RaysNumber :type Integer) (Origin :type Vector) (Direction :type Vector) (ConeAngle :type Float%20%28double-precision%29) (Range :type Float%20%28double-precision%29) (TraceChannel :type ETraceTypeQuery%20Enum :default "TraceTypeQuery1") (DrawDebugType :type EDrawDebugTrace%20Enum :default "None") (DrawTime :type Float%20%28single-precision%29) (TraceColor :type Linear%20Color%20Structure) (ActorsToIgnore :type Array%20of%20Actor%20Object%20References))
  (LocalVariables|SetHalfAngle (/ ConeAngle 2.0))
  (LocalVariables|SetRightVector (Math|Vector|Normalize (Math|Vector|CrossProduct (Math|Vector|VectorUp) Direction)))
  (LocalVariables|SetUpVector (Math|Vector|Normalize (Math|Vector|CrossProduct Direction (LocalVariables|GetRightVector))))
  (for _index (range 1 (/ 360 ConeAngle))
    (bind (_raydirectionoutvalue _allhit) (Raycast|ConeTracebyChannelNotHitImproved RaysNumber Origin Direction (* _index (LocalVariables|GetHalfAngle)) Range TraceChannel DrawDebugType DrawTime TraceColor (LocalVariables|GetRightVector) ActorsToIgnore))
    (if (not _allhit)
      (LocalVariables|SetDirectionsToGo _raydirectionoutvalue)
      (LocalVariables|SetHasADirectionViable true)
      (LocalVariables|SetDirectionToGo (Utilities|Array|Get(acopy) (LocalVariables|GetDirectionsToGo) (Math|Random|RandomInteger (Utilities|Array|LastIndex (LocalVariables|GetDirectionsToGo)))))
      (if (Class|KismetMathLibrary|EqualExactlyVectorVector (LocalVariables|GetDirectionToGo) "0, 0, 0")
        (LocalVariables|SetDirectionToGo (Math|Random|RandomUnitVectorinConeinDegrees Direction (* _index (LocalVariables|GetHalfAngle)))))
      (return (LocalVariables|GetDirectionToGo) (LocalVariables|GetHasADirectionViable))))
  (if (Class|KismetMathLibrary|EqualExactlyVectorVector (LocalVariables|GetDirectionToGo) "0, 0, 0")
    (LocalVariables|SetDirectionToGo (Math|Random|RandomUnitVectorinConeinDegrees Direction (* _index (LocalVariables|GetHalfAngle)))))
  (return (LocalVariables|GetDirectionToGo) (LocalVariables|GetHasADirectionViable)))

(fn GetRandomFloatfromVector
  (params (Vector :type Vector%202D%20Structure))
  (return (Math|Random|RandomFloatinRange (.x Vector) (.y Vector))))

(fn GetRandomIntfromVectorInt
  (params (Vector :type Int%20Vector%20Structure))
  (return (Math|Random|RandomIntegerinRange (.x Vector) (.y Vector))))

(fn MultiplyStruct
  (params (StructFloatCreature :type S%20Float%20Creature%20Mode%20Structure%20%28by%20ref%29) (Multiplier :type Float%20%28double-precision%29))
  (|SetBy-RefVar StructFloatCreature (Utilities|Struct|MakeS_FloatCreatureMode (* (.hunter StructFloatCreature) Multiplier) (* (.prey StructFloatCreature) Multiplier) (* (.neutre StructFloatCreature) Multiplier)))
  (return))

(fn GetVelocity
  (params (Target :type Primitive%20Component%20Object%20Reference))
  (bind _returnvalue (Physics|GetPhysicsLinearVelocity Target "None"))
  (return _returnvalue))

(fn SetLengthConstraint
  (params (PCC_Target :type Physics%20Constraint%20Component%20Object%20Reference%20%28by%20ref%29) (LengthLimit :type Float%20%28single-precision%29))
  (Class|PhysicsConstraintComponent|SetLinearXLimit PCC_Target "LCM_Limited" LengthLimit)
  (Class|PhysicsConstraintComponent|SetLinearYLimit PCC_Target "LCM_Limited" LengthLimit)
  (Class|PhysicsConstraintComponent|SetLinearZLimit PCC_Target "LCM_Limited" LengthLimit)
  (return))

(fn StopPhysicsActor
  (params (ActorToStop :type Actor%20Object%20Reference%20%28by%20ref%29))
  (Utilities|IsValid ActorToStop
    (:Is%20Valid
      (bind _asprimitive_component (Utilities|Casting|CastToPrimitiveComponent (Variables|/Script/Engine.Actor|GetRootComponent ActorToStop)))
      (bind _output_get (LocalVariables|SetPrimitiveRoot _asprimitive_component))
      (Physics|SetSimulatePhysics _output_get false)
      (Physics|SetPhysicsLinearVelocity _output_get "0, 0, 0" false "None")
      (return))))

(fn SetLocationLerp
  (params (CurrentLocation :type Vector) (TargetLocation :type Vector) (InterpolationSpeed :type Float%20%28double-precision%29))
  (return (Math|Vector|Lerp(Vector) CurrentLocation TargetLocation (* InterpolationSpeed (Utilities|Time|GetWorldDeltaSeconds)))))

(fn GetRandomPointinSphere
  (params (Origin :type Vector) (RadiusMinPercent :type Float%20%28double-precision%29) (Radius :type Float%20%28double-precision%29) (SafeRadiusPercent :type Float%20%28double-precision%29))
  (LocalVariables|SetRandomDistance (Math|Random|RandomFloatinRange (* RadiusMinPercent Radius) (- Radius (* Radius SafeRadiusPercent))))
  (LocalVariables|SetRandomDirection (Math|Random|RandomUnitVector))
  (LocalVariables|SetTargetLocation (+ Origin (* (LocalVariables|GetRandomDirection) (LocalVariables|GetRandomDistance))))
  (LocalVariables|SetTargetLocation (+ (LocalVariables|GetTargetLocation) (Math|Vector|NegateVector (* (LocalVariables|GetRandomDirection) (* Radius SafeRadiusPercent)))))
  (return (LocalVariables|GetTargetLocation)))

(fn GetDirectioninCone
  (params (Origin :type Vector) (TargetDirection :type Vector) (UpVector :type Vector) (InputDirection :type Vector%202D%20Structure) (MaxAngle :type Float%20%28double-precision%29) (Range :type Float%20%28double-precision%29) (TraceChannel :type ETraceTypeQuery%20Enum :default "TraceTypeQuery1") (DrawDebugType :type EDrawDebugTrace%20Enum :default "None"))
  (LocalVariables|SetRightVector (Math|Vector|Normalize (Math|Vector|CrossProduct UpVector TargetDirection)))
  (LocalVariables|SetEdgeDirection (Math|Vector|RotateVectorAroundAxis TargetDirection (* MaxAngle (.y InputDirection)) (LocalVariables|GetRightVector)))
  (LocalVariables|SetFinalDirection (Math|Vector|RotateVectorAroundAxis (LocalVariables|GetEdgeDirection) (* MaxAngle (.x InputDirection)) UpVector))
  (return (LocalVariables|GetFinalDirection)))

(fn GetSideBetween2Vec
  (params (Vec1 :type Vector) (Vec2 :type Vector) (NormalPlane :type Vector))
  (return (Math|Vector|DotProduct (Math|Vector|CrossProduct Vec1 Vec2) NormalPlane)))

(fn GetDirectionViaPlan
  (params (Point :type Vector) (PlaneBase :type Vector) (PlaneNormal :type Vector))
  (Rendering|Debug|DrawDebugPoint 0 (Class|KismetMathLibrary|ProjectPointontoPlane Point PlaneBase PlaneNormal) 1e+01 "(R=1.000000,G=1.000000,B=1.000000,A=1.000000)" 0.2))

(fn GetDirectioninConeDynamic
  (params (Origin :type Vector) (TargetDirection :type Vector) (UpVector :type Vector) (InputDirection :type Vector%202D%20Structure) (Range :type Float%20%28double-precision%29) (TraceChannel :type ETraceTypeQuery%20Enum :default "TraceTypeQuery1") (DrawDebugType :type EDrawDebugTrace%20Enum :default "None"))
  (LocalVariables|SetRightVector (Math|Vector|Normalize (Math|Vector|CrossProduct UpVector TargetDirection)))
  (LocalVariables|SetEdgeDirection (Math|Vector|RotateVectorAroundAxis TargetDirection (.y InputDirection) (LocalVariables|GetRightVector)))
  (LocalVariables|SetFinalDirection (Math|Vector|RotateVectorAroundAxis (LocalVariables|GetEdgeDirection) (.x InputDirection) UpVector))
  (return (LocalVariables|GetFinalDirection)))

(fn SpawnNSonSocket
  (params (TargetSKM :type Skeletal%20Mesh%20Object%20Reference) (NSToSpawn :type Niagara%20System%20Object%20Reference) (SocketName :type Name))
  (bind (_outtransform _outboneindex _outindex _returnvalue) (Class|SkinnedAsset|FindSocketInfo TargetSKM SocketName))
  (Utilities|IsValid _returnvalue
    (:Is%20Valid
      (Niagara|SpawnSystematLocation TargetSKM NSToSpawn (.location _outtransform) (.rotation _outtransform) (.scale _outtransform)))
    (:Is%20Not%20Valid
      (Development|PrintText 0 "Socket Not Found" true true "(R=1.000000,G=0.000000,B=0.038797,A=1.000000)" 5.0)))
  (return))

(fn GetDifferenceTime
  (params (PreviousTime :type Timecode%20Structure) (CurrentTime :type Timecode%20Structure))
  (bind (_hours _minutes _seconds) (Utilities|Struct|BreakTimecode CurrentTime))
  (bind (_hours_2 _minutes_2 _seconds_2) (Utilities|Struct|BreakTimecode PreviousTime))
  (bind _output_get (LocalVariables|SetOutTimeCode (Utilities|Struct|MakeTimecode (- _hours_2 _hours) (- _minutes_2 _minutes) (- _seconds_2 _seconds) 0 false)))
  (return _output_get))

(fn GetDifferenceMinutes
  (params (PreviousTime :type Timecode%20Structure) (CurrentTime :type Timecode%20Structure))
  (bind _out_timecode (Time|GetDifferenceTime PreviousTime CurrentTime))
  (bind (_hours _minutes) (Utilities|Struct|BreakTimecode _out_timecode))
  (return (+ (* _hours 60) _minutes)))

(fn GetDifferenceSeconds
  (params (PreviousTime :type Timecode%20Structure) (CurrentTime :type Timecode%20Structure))
  (bind _out_timecode (Time|GetDifferenceTime PreviousTime CurrentTime))
  (bind (_hours _minutes _seconds) (Utilities|Struct|BreakTimecode _out_timecode))
  (return (+ (+ (* _hours 360) (* _minutes 60)) _seconds)))

(fn GetRandomFloatwithGap
  (params (GapMin :type Float%20%28double-precision%29) (Max :type Float%20%28double-precision%29))
  (LocalVariables|SetRandomFloat (Math|Random|RandomFloatinRange GapMin Max))
  (if (Math|Random|RandomBool)
    (Math|Float|DecrementFloat (LocalVariables|GetRandomFloat)
      (:%20%20
        _)))
  (return (LocalVariables|GetRandomFloat)))