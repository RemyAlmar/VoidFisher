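; BP_flow is a spline-shaped flow actor that acts on the player test camera controller while it overlaps.
; Construction builds spline mesh segments from a collider mesh along each spline span and binds the spline to a Niagara system, rebound at BeginPlay.
; Overlap events track the player, and Tick sends it the spline through FlowStartMessage while inside.
; A helper estimates spline bounds by sampling, but nothing here calls it.
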(event EventBeginPlay
  (CallFunction|NiagaraInitialize))

(event Collision|EventActorBeginOverlap
  (params (OtherActor :type Actor%20Object%20Reference))
  (if (== (Utilities|GetClass OtherActor) "/Game/Blueprints/Game/Player/Controllers/BP_PlayerTestCamController.BP_PlayerTestCamController_C")
    (Variables|Default|SetPlayer OtherActor)
    (Variables|Default|SetPlayerIsInFlow true)))

(event EventTick
  (params (DeltaSeconds :type Float%20%28single-precision%29))
  (if (Variables|Default|GetPlayerIsInFlow)
    (Class|BPIEnvironmentInfluence|FlowStart(Message) (Variables|Default|GetPlayer) (Variables|Default|GetSpline))))

(event Collision|EventActorEndOverlap
  (params (OtherActor :type Actor%20Object%20Reference))
  (if (== (Utilities|GetClass OtherActor) "/Game/Blueprints/Game/Player/Controllers/BP_PlayerTestCamController.BP_PlayerTestCamController_C")
    (Variables|Default|SetPlayerIsInFlow false)))

(fn ConstructionScript
  (bind _scale (Variables|Default|GetScale))
  (bind _spline (Variables|Default|GetSpline))
  (Utilities|FlowControl|Sequence
    (:then_0
      (CallFunction|NiagaraInitialize))
    (:then_1
      (for _index (range 0 (- (Spline|GetNumberOfSplinePoints (Variables|Default|GetSpline)) 2))
        (bind _returnvalue (AddComponent|AddSplineMeshComponent false))
        (Components|StaticMesh|SetStaticMesh _returnvalue (Variables|Default|GetColliderMesh))
        (SplineMesh|SetStartScale _returnvalue _scale true :!class /Script/Engine.SplineMeshComponent)
        (SplineMesh|SetEndScale _returnvalue _scale true :!class /Script/Engine.SplineMeshComponent)
        (SplineMesh|SetStartandEnd _returnvalue (Spline|GetLocationatSplinePoint _spline _index "Local") (Spline|GetTangentatSplinePoint _spline _index "Local") (Spline|GetLocationatSplinePoint _spline (+ _index 1) "Local") (Spline|GetTangentatSplinePoint _spline (+ _index 1) "Local") true :!class /Script/Engine.SplineMeshComponent)))))

(fn NiagaraInitialize
  (Niagara|SetNiagaraVariable(Object) (Variables|Default|GetNiagara) "Splines" (Variables|Default|GetSpline)))

(fn EstimateSplineBounds
  (bind _boundsoffset (Variables|Default|GetBoundsOffset))
  (bind _output_get (LocalVariables|SetThisMin "100000000000.000000,100000000000.000000,100000000000.000000"))
  (LocalVariables|SetThisMax (* _output_get -1.0))
  (for _index (range 0 99)
    (bind _output_get_2 (LocalVariables|SetThisSample (- (Spline|GetLocationatTime (Variables|Default|GetSpline) (/ _index 100) "Local" true) (Transformation|GetActorLocation))))
    (LocalVariables|SetThisMin (Math|Vector|MakeVector (Math|Float|Min(Float) (.X (Math|Vector|BreakVector _output_get_2)) (.X (Math|Vector|BreakVector (LocalVariables|GetThisMin)))) (Math|Float|Min(Float) (.Y (Math|Vector|BreakVector _output_get_2)) (.Y (Math|Vector|BreakVector (LocalVariables|GetThisMin)))) (Math|Float|Min(Float) (.Z (Math|Vector|BreakVector _output_get_2)) (.Z (Math|Vector|BreakVector (LocalVariables|GetThisMin))))))
    (LocalVariables|SetThisMax (Math|Vector|MakeVector (Math|Float|Max(Float) (.X (Math|Vector|BreakVector _output_get_2)) (.X (Math|Vector|BreakVector (LocalVariables|GetThisMax)))) (Math|Float|Max(Float) (.Y (Math|Vector|BreakVector _output_get_2)) (.Y (Math|Vector|BreakVector (LocalVariables|GetThisMax)))) (Math|Float|Max(Float) (.Z (Math|Vector|BreakVector _output_get_2)) (.Z (Math|Vector|BreakVector (LocalVariables|GetThisMax)))))))
  (return (+ (LocalVariables|GetThisMin) _boundsoffset) (- (LocalVariables|GetThisMax) _boundsoffset)))