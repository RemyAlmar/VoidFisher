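; Water flow actor that drives ten Niagara particle and ribbon effects, each fed its own spline.
; Both the construction script and BeginPlay initialize every spline and Niagara pair through NiagaraInitialize.
; That function sizes the box and fixed system bounds from a shared Extent, passes in the spline, then pushes shared color, force, forward, magnet and global settings structs as Niagara variables.
; FlowStart is an empty stub.
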(event EventBeginPlay
  (CallFunction|NiagaraInitialize (Variables|Default|GetSpline) (Variables|Default|GetNiagara))
  (CallFunction|NiagaraInitialize (Variables|Default|GetSpline1) (Variables|Default|GetNiagara1))
  (CallFunction|NiagaraInitialize (Variables|Default|GetSpline2) (Variables|Default|GetNiagara2))
  (CallFunction|NiagaraInitialize (Variables|Default|GetSpline3) (Variables|Default|GetNiagara3))
  (CallFunction|NiagaraInitialize (Variables|Default|GetSpline4) (Variables|Default|GetNiagara4))
  (CallFunction|NiagaraInitialize (Variables|Default|GetSpline5) (Variables|Default|GetNiagara5))
  (CallFunction|NiagaraInitialize (Variables|Default|GetSpline6) (Variables|Default|GetNiagara6))
  (CallFunction|NiagaraInitialize (Variables|Default|GetSpline7) (Variables|Default|GetNiagara7))
  (CallFunction|NiagaraInitialize (Variables|Default|GetSpline8) (Variables|Default|GetNiagara8))
  (CallFunction|NiagaraInitialize (Variables|Default|GetSpline9) (Variables|Default|GetNiagara9)))

(fn ConstructionScript
  (CallFunction|NiagaraInitialize (Variables|Default|GetSpline) (Variables|Default|GetNiagara))
  (CallFunction|NiagaraInitialize (Variables|Default|GetSpline1) (Variables|Default|GetNiagara1))
  (CallFunction|NiagaraInitialize (Variables|Default|GetSpline2) (Variables|Default|GetNiagara2))
  (CallFunction|NiagaraInitialize (Variables|Default|GetSpline3) (Variables|Default|GetNiagara3))
  (CallFunction|NiagaraInitialize (Variables|Default|GetSpline4) (Variables|Default|GetNiagara4))
  (CallFunction|NiagaraInitialize (Variables|Default|GetSpline5) (Variables|Default|GetNiagara5))
  (CallFunction|NiagaraInitialize (Variables|Default|GetSpline6) (Variables|Default|GetNiagara6))
  (CallFunction|NiagaraInitialize (Variables|Default|GetSpline7) (Variables|Default|GetNiagara7))
  (CallFunction|NiagaraInitialize (Variables|Default|GetSpline8) (Variables|Default|GetNiagara8))
  (CallFunction|NiagaraInitialize (Variables|Default|GetSpline9) (Variables|Default|GetNiagara9)))

(fn NiagaraInitialize
  (params (Spline :type Object%20Object%20Reference) (Niagara :type Niagara%20Component%20Object%20Reference))
  (bind _extent (Variables|Bounds|GetExtent))
  (Components|Box|SetBoxExtent (Variables|Default|GetBox) _extent false)
  (Class|NiagaraComponent|SetSystemFixedBounds Niagara (Class|KismetMathLibrary|MakeBoxwithOrigin (Transformation|GetActorLocation) _extent))
  (Niagara|SetNiagaraVariable(Object) Niagara "Splines" Spline)
  (|SetColorVariables Niagara)
  (|SetForceVariables Niagara)
  (|SetForwardVariables Niagara)
  (|SetMagnetVariables Niagara)
  (|SetGlobalVariables Niagara))

(fn FlowStart
  (params (Spline :type Spline%20Component%20Object%20Reference) (BaseSpeed :type Float%20%28double-precision%29) (SlugSpeed :type Float%20%28double-precision%29) (SubsonicSpeed :type Float%20%28double-precision%29) (MagnetStrength :type Float%20%28double-precision%29) (Damping :type Float%20%28double-precision%29)))