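; BP_Gravity is a component that pulls nearby physics-simulating components toward the center of a gravity sphere.
; Outer and inner sphere overlaps maintain the influenced list, with the inner sphere suspending attraction.
; Each tick adds velocity toward the center, scaled by gravity force and the radius gap over distance to an offset "ground" point.
; Radii scale with the owner's largest axis at BeginPlay, and debug prints remain.
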(event Custom|OnBeginOverlapAttracted
  (params (OverlappedComponent :type Primitive%20Component%20Object%20Reference) (OtherActor :type Actor%20Object%20Reference) (OtherComp :type Primitive%20Component%20Object%20Reference) (OtherBodyIndex :type Integer) (bFromSweep :type Boolean) (SweepResult :type Hit%20Result%20Structure%20%28by%20ref%29))
  (Development|PrintString "Begin Overlap")
  (if (Physics|IsSimulatingPhysics OtherComp "None")
    (Utilities|Array|AddUnique (Variables|CustomPhysics|GetListActorCompInfluenced) OtherComp)))

(event Custom|OnEndOverlapAttracted
  (params (OverlappedComponent :type Primitive%20Component%20Object%20Reference) (OtherActor :type Actor%20Object%20Reference) (OtherComp :type Primitive%20Component%20Object%20Reference) (OtherBodyIndex :type Integer))
  (Development|PrintString "End Overlap" true true "(R=0.890202,G=0.000000,B=1.000000,A=1.000000)")
  (if (Utilities|Array|ContainsItem (Variables|CustomPhysics|GetListActorCompInfluenced) OtherComp)
    (Utilities|Array|RemoveItem (Variables|CustomPhysics|GetListActorCompInfluenced) OtherComp)))

(event Custom|OnBeginOverlapStopAttracted
  (params (OverlappedComponent :type Primitive%20Component%20Object%20Reference) (OtherActor :type Actor%20Object%20Reference) (OtherComp :type Primitive%20Component%20Object%20Reference) (OtherBodyIndex :type Integer) (bFromSweep :type Boolean) (SweepResult :type Hit%20Result%20Structure%20%28by%20ref%29))
  (if (Utilities|Array|ContainsItem (Variables|CustomPhysics|GetListActorCompInfluenced) OtherComp)
    (Utilities|Array|RemoveItem (Variables|CustomPhysics|GetListActorCompInfluenced) OtherComp)))

(event Custom|OnEndOverlapStopAttracted
  (params (OverlappedComponent :type Primitive%20Component%20Object%20Reference) (OtherActor :type Actor%20Object%20Reference) (OtherComp :type Primitive%20Component%20Object%20Reference) (OtherBodyIndex :type Integer))
  (Development|PrintString "Begin Overlap")
  (if (Physics|IsSimulatingPhysics OtherComp "None")
    (Utilities|Array|AddUnique (Variables|CustomPhysics|GetListActorCompInfluenced) OtherComp)))

(event EventBeginPlay
  (Collision|BindEventtoOnComponentBeginOverlap (Variables|Default|GetGravityInfluenceArea) (EventDispatchers|CreateEvent :!event Custom|OnBeginOverlapAttracted))
  (Collision|BindEventtoOnComponentEndOverlap (Variables|Default|GetGravityInfluenceArea) (EventDispatchers|CreateEvent :!event Custom|OnEndOverlapAttracted))
  (Collision|BindEventtoOnComponentBeginOverlap (Variables|Default|GetStopGravityInfluenceArea) (EventDispatchers|CreateEvent :!event Custom|OnBeginOverlapStopAttracted))
  (Collision|BindEventtoOnComponentEndOverlap (Variables|Default|GetStopGravityInfluenceArea) (EventDispatchers|CreateEvent :!event Custom|OnEndOverlapStopAttracted))
  (Variables|Radius|SetInfluenceRadius (CallFunction|SetRadiusbyScale (Variables|/Script/Engine.SphereComponent|GetSphereRadius (Variables|Default|GetGravityInfluenceArea))))
  (Variables|Radius|SetStopInfluenceRadius (CallFunction|SetRadiusbyScale (Variables|/Script/Engine.SphereComponent|GetSphereRadius (Variables|Default|GetStopGravityInfluenceArea)))))

(event EventTick
  (params (DeltaSeconds :type Float%20%28single-precision%29))
  (if (Utilities|Array|IsNotEmpty (Variables|CustomPhysics|GetListActorCompInfluenced))
    (CallFunction|AttractAllActorsinInfluence)))

(fn SetInfluenceSphere
  (params (GravityInfluenceArea :type Sphere%20Component%20Object%20Reference) (StopGravityInfluenceArea :type Sphere%20Component%20Object%20Reference))
  (Variables|Default|SetGravityInfluenceArea GravityInfluenceArea)
  (Variables|Default|SetStopGravityInfluenceArea StopGravityInfluenceArea))

(fn ChangeRadiusInfluence
  (params (NewRadius :type Float%20%28double-precision%29))
  (Components|Sphere|SetSphereRadius (Variables|Default|GetGravityInfluenceArea) NewRadius true))

(fn AttractAllActorsinInfluence
  (for _array_element (Variables|CustomPhysics|GetListActorCompInfluenced)
    (Utilities|IsValid (Components|GetOwner _array_element)
      (:Is%20Valid
        (bind _output_get (LocalVariables|SetAttractedDirection (Math|Vector|Normalize (- (Transformation|GetWorldLocation (Variables|Default|GetGravityInfluenceArea)) (Transformation|GetWorldLocation _array_element)))))
        (Development|PrintString (Utilities|String|ToString(Float) (* (Variables|CustomPhysics|GetGravityForce) (/ (CallFunction|GetDistanceMax) (Math|Vector|Distance(Vector) (CallFunction|GetGroundLocation (LocalVariables|GetAttractedDirection)) (Transformation|GetWorldLocation _array_element))))) true true "(R=0.819650,G=1.000000,B=0.000000,A=1.000000)")
        (Physics|SetPhysicsLinearVelocity _array_element (* _output_get (* (Variables|CustomPhysics|GetGravityForce) (/ (CallFunction|GetDistanceMax) (Math|Vector|Distance(Vector) (CallFunction|GetGroundLocation (LocalVariables|GetAttractedDirection)) (Transformation|GetWorldLocation _array_element))))) true "None"))))
  (return))

(fn SetRadiusbyScale
  (params (OriginRadius :type Float%20%28double-precision%29))
  (bind _returnvalue (Components|GetOwner))
  (bind _returnvalue_2 (Transformation|GetActorScale3D _returnvalue))
  (return (* OriginRadius (Math|Float|Max(Float) (Math|Float|Max(Float) (.x _returnvalue_2) (.y _returnvalue_2)) (.z _returnvalue_2)))))

(fn GetGroundLocation
  (params (NormalizeDirection :type Vector))
  (return (+ (Transformation|GetActorLocation (Components|GetOwner)) (* NormalizeDirection (Variables|Radius|GetStopInfluenceRadius)))))

(fn GetDistanceMax
  (return (- (Variables|Radius|GetInfluenceRadius) (Variables|Radius|GetStopInfluenceRadius))))