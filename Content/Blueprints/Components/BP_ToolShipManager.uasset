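; BP_ToolShipManager is a component that manages the ship's tools, keeping them in a map by enum key and tracking a single active one.
; Tools are registered through AddTool, unlocked by clearing their lock flag, and used through the currently active entry.
; ToggleTool closes the requested tool if already active, otherwise SwitchTool deactivates the current one and activates the new one.
; Closing resets the active key to a fixed enum value.
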(fn OpenTool
  (params (ToolToOpen :type E_ToolShip%20Enum :default "NewEnumerator0"))
  (Default|Active (.Value (Utilities|Map|Find (Variables|Default|GetToolList) ToolToOpen)))
  (Variables|Default|SetCurrentToolActive ToolToOpen))

(fn CloseTool
  (params (ToolToClosed :type E_ToolShip%20Enum :default "NewEnumerator0"))
  (Default|Deactive (.Value (Utilities|Map|Find (Variables|Default|GetToolList) ToolToClosed)))
  (Variables|Default|SetCurrentToolActive "NewEnumerator3"))

(fn UnlockTool
  (params (ToolToUnlock :type E_ToolShip%20Enum :default "NewEnumerator3"))
  (Variables|/Game/Blueprints/Player/Tools/BP_ToolBase.BP_ToolBase_C|SetIsLock (.Value (Utilities|Map|Find (Variables|Default|GetToolList) ToolToUnlock)) false))

(fn UseTool
  (Default|Use (.Value (Utilities|Map|Find (Variables|Default|GetToolList) (Variables|Default|GetCurrentToolActive)))))

(fn ToggleTool
  (params (NextTool :type E_ToolShip%20Enum :default "NewEnumerator3"))
  (if (Private|AlreadyActive NextTool)
    (Private|CloseTool NextTool)
    (else
      (Private|SwitchTool NextTool))))

(fn SwitchTool
  (params (NewTool :type E_ToolShip%20Enum :default "NewEnumerator0"))
  (Private|CloseTool (Variables|Default|GetCurrentToolActive))
  (Private|OpenTool NewTool))

(fn AlreadyActive
  (params (ToolToActive :type E_ToolShip%20Enum :default "NewEnumerator3"))
  (return (Utilities|Enum|Equal(Enum) ToolToActive (Variables|Default|GetCurrentToolActive))))

(fn AddTool
  (params (Key :type E_ToolShip%20Enum%20%28by%20ref%29 :default "NewEnumerator3") (Value :type BP%20Tool%20Base%20Object%20Reference%20%28by%20ref%29))
  (Utilities|Map|Add (Variables|Default|GetToolList) Key Value))