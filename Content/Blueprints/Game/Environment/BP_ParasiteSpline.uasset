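; BP_ParasiteSpline is an environment spline actor that lays a chosen static mesh along an editable path.
; Its construction script adds one spline mesh per point pair, fitted to local positions and tangents.
; Segment scale is either global, separate start and end values, or random per end, rerolled on construction and not matched between neighbors.
; ResetVariables restores global scaling and unit values for start, end and mesh scale.
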(fn ConstructionScript
  (bind _scale (Variables|Parasite|GetScale))
  (bind _meshscale (Variables|Parasite|GetMeshScale))
  (bind _maxscale (Variables|RandomScale|GetMaxScale))
  (bind _minscale (Variables|RandomScale|GetMinScale))
  (bind _returnvalue (Math|Random|RandomFloatinRange _minscale _maxscale))
  (bind _returnvalue_2 (* _scale _meshscale))
  (for _index (range 0 (- (Spline|GetNumberOfSplinePoints (Variables|Default|GetSpline)) 2))
    (LocalVariables|SetID _index)
    (bind _returnvalue_3 (AddComponent|AddSplineMeshComponent false))
    (Components|StaticMesh|SetStaticMesh _returnvalue_3 (Variables|Parasite|GetStaticMesh))
    (SplineMesh|SetForwardAxis _returnvalue_3 (Variables|Parasite|GetForwardAxis) true)
    (bind (_location _tangent) (CallFunction|GetStartPos/Tangent (LocalVariables|GetID)))
    (bind (_location_2 _tangent_2) (CallFunction|GetEndPos/Tangent (LocalVariables|GetID)))
    (SplineMesh|SetStartandEnd _returnvalue_3 _location _tangent _location_2 _tangent_2 true :!class /Script/Engine.SplineMeshComponent)
    (if (not (Variables|RandomScale|GetRandomScale))
      (if (Variables|Parasite|GetGlobalScale)
        (SplineMesh|SetStartScale _returnvalue_3 _returnvalue_2 true :!class /Script/Engine.SplineMeshComponent)
        (SplineMesh|SetEndScale _returnvalue_3 _returnvalue_2 true :!class /Script/Engine.SplineMeshComponent)
        (else
          (SplineMesh|SetStartScale _returnvalue_3 (Math|Conversions|ToVector2D(Vector) (Variables|Parasite|GetStart%20Scale)) true :!class /Script/Engine.SplineMeshComponent)
          (SplineMesh|SetEndScale _returnvalue_3 (Math|Conversions|ToVector2D(Vector) (Variables|Parasite|GetEnd%20Scale)) true :!class /Script/Engine.SplineMeshComponent)))
      (else
        (SplineMesh|SetStartScale _returnvalue_3 (Math|Conversions|ToVector2D(Vector) _returnvalue) true :!class /Script/Engine.SplineMeshComponent)
        (SplineMesh|SetEndScale _returnvalue_3 (Math|Conversions|ToVector2D(Vector) _returnvalue) true :!class /Script/Engine.SplineMeshComponent)))))

(fn GetStartPos/Tangent
  (params (ID :type Integer))
  (bind _spline (Variables|Default|GetSpline))
  (return (Spline|GetLocationatSplinePoint _spline ID "Local") (Spline|GetTangentatSplinePoint _spline ID "Local")))

(fn GetEndPos/Tangent
  (params (ID :type Integer))
  (bind _returnvalue (+ ID 1))
  (bind _spline (Variables|Default|GetSpline))
  (return (Spline|GetLocationatSplinePoint _spline _returnvalue "Local") (Spline|GetTangentatSplinePoint _spline _returnvalue "Local")))

(fn ResetVariables
  (Variables|Parasite|SetEnd%20Scale 1.0)
  (Variables|Parasite|SetStart%20Scale 1.0)
  (Variables|Parasite|SetGlobalScale true)
  (Variables|Parasite|SetMeshScale 1.0))