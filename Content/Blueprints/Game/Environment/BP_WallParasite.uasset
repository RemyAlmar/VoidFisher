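; BP_WallParasite is a wall that stays in place until every actor in its Parasite list is destroyed.
; Construction sets the wall mesh, and both construction and BeginPlay rebind each parasite's OnDestroyed event.
; Each destroyed parasite leaves the list, and an empty list triggers Dissolve.
; Dissolve disables collision, drives a dynamic material's dissolve parameter with a Timeline, then destroys the wall actor.
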(event Custom|Parasite_ED_OnDestroyActor_Event
  (params (TargetToDestroy :type Actor%20Object%20Reference))
  (Utilities|Array|RemoveItem (Variables|Parasite|GetParasite) TargetToDestroy)
  (if (Utilities|Array|IsEmpty (Variables|Parasite|GetParasite))
    (CallFunction|Dissolve)))

(event Custom|Dissolve
  (Collision|SetCollisionEnabled (Variables|Default|GetWall) "NoCollision")
  (bind _alpha (Timeline|Timeline PlayFromStart)
    (:Update
      (Rendering|Material|SetScalarParameterValue (Variables|Default|GetMaterial) "Dissolve" _alpha :!class /Script/Engine.MaterialInstanceDynamic))
    (:Finished
      (Actor|DestroyActor))))

(event EventBeginPlay
  (bind _returnvalue (Rendering|Material|CreateDynamicMaterialInstance (Variables|Default|GetWall) 0 "/Game/VFX/Materials/Parasite/MI_BlackRockPALEnter.MI_BlackRockPALEnter" "None" :!class /Script/Engine.PrimitiveComponent))
  (Variables|Default|SetMaterial _returnvalue)
  (for _array_element (Variables|Parasite|GetParasite)
    (Game|UnbindEventfromOnDestroyed _array_element (EventDispatchers|CreateEvent :!event Custom|Parasite_ED_OnDestroyActor_Event))
    (Game|BindEventtoOnDestroyed _array_element (EventDispatchers|CreateEvent :!event Custom|Parasite_ED_OnDestroyActor_Event))))

(fn ConstructionScript
  (Components|StaticMesh|SetStaticMesh (Variables|Default|GetWall) (Variables|Parasite|GetWallMesh))
  (for _array_element (Variables|Parasite|GetParasite)
    (Game|UnbindEventfromOnDestroyed _array_element (EventDispatchers|CreateEvent :!event Custom|Parasite_ED_OnDestroyActor_Event))
    (Game|BindEventtoOnDestroyed _array_element (EventDispatchers|CreateEvent :!event Custom|Parasite_ED_OnDestroyActor_Event))))