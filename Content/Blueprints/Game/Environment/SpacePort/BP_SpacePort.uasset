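; Spaceport actor that opens a ship HUD menu when the player enters its trigger box and respawns them at an exit point afterwards.
; One tick after BeginPlay it binds to that menu's close dispatcher, and closing respawns the player through the GameInstance only if they entered this port.
; ActiveOverlap switches the box's overlap events on or off and fires the matching open or close dispatcher.
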(event OnComponentBeginOverlap(Box)
  (params (OverlappedComponent :type Primitive%20Component%20Object%20Reference) (OtherActor :type Actor%20Object%20Reference) (OtherComp :type Primitive%20Component%20Object%20Reference) (OtherBodyIndex :type Integer) (bFromSweep :type Boolean) (SweepResult :type Hit%20Result%20Structure%20%28by%20ref%29))
  (bind _asbp_player_refonte (Utilities|Casting|CastToBP_PlayerRefonte OtherActor))
  (bind _output_get (Variables|Default|SetPlayerRefonte _asbp_player_refonte))
  (Default|ClearAllExceptMenuTarget (Variables|/Game/Blueprints/Game/Player/Controllers/BP_PlayerRefonte.BP_PlayerRefonte_C|GetHUD_Ship _output_get) "NewEnumerator9")
  (Default|ToggleWidget (Variables|/Game/Blueprints/Game/Player/Controllers/BP_PlayerRefonte.BP_PlayerRefonte_C|GetHUD_Ship _output_get) "NewEnumerator9")
  (Variables|Default|SetIsInspaceport true))

(event Custom|CloseWidgetSpaceport
  (bind _exitposition (Variables|Default|GetExitPosition))
  (bind _returnvalue (Transformation|GetWorldTransform _exitposition))
  (if (Variables|Default|GetIsInspaceport)
    (Default|RespawnPlayer (Variables|Default|GetGameInstance) (Math|Transform|MakeTransform (.location _returnvalue) (.rotation _returnvalue) "1.000000,1.000000,1.000000"))
    (Variables|Default|SetIsInspaceport false)))

(event EventBeginPlay
  (bind _asbp_game_instance (Utilities|Casting|CastToBP_GameInstance (Game|GetGameInstance)))
  (bind _output_get (Variables|Default|SetGameInstance _asbp_game_instance))
  (Utilities|FlowControl|DelayUntilNextTick)
  (EventDispatchers|BindEventtoEDonCloseMenu (.Value (Utilities|Map|Find (Variables|/Game/Blueprints/Widgets/HUD/BP_HUD_Ship.BP_HUD_Ship_C|GetMenuWidgetToSwitch (Variables|/Game/Blueprints/Game/Player/Controllers/BP_PlayerRefonte.BP_PlayerRefonte_C|GetHUD_Ship (Variables|/Game/Blueprints/Data/BP_GameInstance.BP_GameInstance_C|GetPlayer _output_get))) "NewEnumerator9")) (EventDispatchers|CreateEvent :!event Custom|CloseWidgetSpaceport)))

(fn ConstructionScript)

(fn ActiveOverlap
  (params (Active :type Boolean))
  (bind _output_get (Variables|/Script/Engine.PrimitiveComponent|SetbGenerateOverlapEvents (Variables|Default|GetBox) Active))
  (if _output_get
    (Default|CallEDonOpen)
    (else
      (Default|CallEDonClose))))