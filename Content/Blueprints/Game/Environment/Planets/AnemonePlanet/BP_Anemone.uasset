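; Anemone planet environment actor with Niagara water flows that follow splines and carry positional sound.
; Construction Script and BeginPlay pass each of three splines to its Niagara system as an object variable.
; BeginPlay also creates one audio component per spline component and caches the player pawn.
; While the player is within a set distance of the actor, Tick moves each sound to its spline's closest point to the player.
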(event EventBeginPlay
  (Utilities|FlowControl|Sequence
    (:then_0
      (Niagara|SetNiagaraVariable(Object) (Variables|Default|GetNS_StartWaterFlow) "Spline" (Variables|Spline|GetSpline))
      (Niagara|SetNiagaraVariable(Object) (Variables|Default|GetNS_StartWaterFlow1) "Spline" (Variables|Spline|GetSpline1))
      (Niagara|SetNiagaraVariable(Object) (Variables|Default|GetNS_StartWaterFlow2) "Spline" (Variables|Spline|GetSpline2)))
    (:then_1
      ;[1 1 1] Création de list pour la musique et les spline
      (bind _output_get (Variables|Default|SetSplineList (Actor|GetComponentsByClass "/Script/Engine.SplineComponent")))
      (for _array_element _output_get
        (bind _returnvalue (AddComponent|AddAudioComponent false))
        (Utilities|Array|Add (Variables|Default|GetAudioList) _returnvalue)))
    (:then_2
      (bind _asbp_player_refonte (Utilities|Casting|CastToBP_PlayerRefonte (Game|Player|GetPlayerPawn 0)))
      (Variables|Default|SetPlayer _asbp_player_refonte))))

(event EventTick
  (params (DeltaSeconds :type Float%20%28single-precision%29))
  ;[1 1 1] Rajoute un son sur les points de spline les plus proche du joueur
  (bind _player (Variables|Default|GetPlayer)
    (:then
      (if (<= (Math|Vector|Distance(Vector) (Transformation|GetActorLocation _player) (Transformation|GetActorLocation)) (Variables|Default|GetDistanceMinToMoveSound*))
        (for (_array_element _array_index) (Variables|Default|GetSplineList)
          (Transformation|SetWorldLocation (Utilities|Array|Get(acopy) (Variables|Default|GetAudioList) _array_index) (CallFunction|GetClosestLocationonSpline (Transformation|GetActorLocation _player) _array_element) false false))))
    (:else)))

(fn ConstructionScript
  (Niagara|SetNiagaraVariable(Object) (Variables|Default|GetNS_StartWaterFlow) "Spline" (Variables|Spline|GetSpline))
  (Niagara|SetNiagaraVariable(Object) (Variables|Default|GetNS_StartWaterFlow1) "Spline" (Variables|Spline|GetSpline1))
  (Niagara|SetNiagaraVariable(Object) (Variables|Default|GetNS_StartWaterFlow2) "Spline" (Variables|Spline|GetSpline2)))

(fn GetClosestLocationonSpline
  (params (TargetLocation :type Vector%20%28by%20ref%29) (Target :type Spline%20Component%20Object%20Reference))
  (return (Spline|GetLocationatDistanceAlongSpline Target (Class|SplineComponent|GetDistanceAlongSplineatLocation Target TargetLocation "World") "World")))