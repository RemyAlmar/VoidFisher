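; Environment actor base driven by a state manager component, which it initializes from a list of state classes and updates every tick.
; Interface start, update, quit and state-change calls are relayed through event dispatchers.
; Activation toggles collision, all actor components and tracked VFX, the latter via their "Kill Particles" variable.
; With AutoRotate on, construction aligns the actor's up axis to the nearest surface normal found by cone traces.
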(event Custom|ED_OnStart_Event
  (Default|CallEDonStart))

(event Custom|ED_OnUpdate_Event
  (params (DeltaSeconds :type Float%20%28double-precision%29))
  (Default|CallEDonUpdate DeltaSeconds))

(event Custom|ED_OnQuit_Event
  (Default|CallEDonQuit))

(event Custom|ED_ChangeState_Event
  (params (TargetState :type Byte))
  (Default|CallEDChangeState TargetState))

(event Custom|ED_OnActivation_Event
  (params (Active :type Boolean))
  (Collision|SetActorEnableCollision Active)
  (Array|ActiveAllActorComponentbyClass "/Script/Engine.ActorComponent" Active)
  (Array|ParticleSystem|ActiveAllParticleSystem Active))

(event EventTick
  (params (DeltaSeconds :type Float%20%28single-precision%29))
  (Default|IUpdate (Variables|Default|GetBPC_StateManager) DeltaSeconds))

(event EventIStart
  (CallFunction|EDonStartEvent))

(event EventIUpdate
  (params (DeltaSeconds :type Float%20%28double-precision%29))
  (CallFunction|EDonUpdateEvent DeltaSeconds))

(event EventIQuit
  (CallFunction|EDonQuitEvent))

(event EventIChangeState
  (params (TargetState :type Byte :default 0))
  (CallFunction|EDChangeStateEvent TargetState))

(event EventBeginPlay
  (Default|Initialize (Variables|Default|GetBPC_StateManager) (Variables|Default|GetList%20States%20Class))
  (EventDispatchers|BindEventtoEDonActivation (EventDispatchers|CreateEvent :!event Custom|ED_OnActivation_Event)))

(fn ConstructionScript
  (if (Variables|Param|GetAutoRotate)
    (Param|RotatebyNearestNormal))
  (|CallParentFunction))

(fn AddParticleSystem
  (params (NewItem :type Niagara%20Component%20Object%20Reference%20%28by%20ref%29))
  (Utilities|Array|AddUnique (Variables|Default|GetListVFXSpawned) NewItem))

(fn RemoveParticleSystem
  (params (Item :type Niagara%20Component%20Object%20Reference%20%28by%20ref%29))
  (Utilities|Array|RemoveItem (Variables|Default|GetListVFXSpawned) Item))

(fn RemoveAllParticleSystem
  (bind _listvfxspawned (Variables|Default|GetListVFXSpawned))
  (for _array_element _listvfxspawned
    (Utilities|Array|RemoveItem _listvfxspawned _array_element)
    (Components|DestroyComponent _array_element))
  (return))

(fn ActiveActorComponent
  (params (Target :type Actor%20Component%20Object%20Reference) (bNewActive :type Boolean))
  (Components|Activation|SetActive Target bNewActive false))

(fn ActiveAllActorComponentbyClass
  (params (ComponentClass :type Actor%20Component%20Class%20Reference) (NewActive :type Boolean))
  (for _array_element (Actor|GetComponentsByClass self ComponentClass)
    (Components|Activation|SetActive _array_element NewActive false)
    (Development|PrintText (Utilities|Text|ToText(String) (Utilities|GetDisplayName _array_element))))
  (return))

(fn ActiveAllParticleSystem
  (params (bNewActive :type Boolean))
  (for _array_element (Variables|Default|GetListVFXSpawned)
    (Class|NiagaraComponent|SetVariableBool _array_element "Kill Particles" (not bNewActive)))
  (return))

(fn RotatebyNearestNormal
  (bind (_nearesthit _hasahit) (CallFunction|GetNearestHitLocationfromSphereRadius (Variables|Param|GetAccuracySnap) (Transformation|GetActorLocation) (Transformation|GetActorUpVector) (Transformation|GetActorRightVector) 1e+01 (Variables|Param|GetRangeSnap) 360 "TraceTypeQuery3" "None" 3.0 "(R=0.000000,G=0.537358,B=1.000000,A=1.000000)"))
  (if _hasahit
    (LocalVariables|SetNextRotation (Math|Rotator|MakeRotfromZ (.Normal (Collision|BreakHitResult _nearesthit))))
    (else
      (LocalVariables|SetNextRotation (Transformation|GetActorRotation))))
  (Transformation|SetActorRotation (LocalVariables|GetNextRotation))
  (return))