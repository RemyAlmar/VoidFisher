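; BP_Hideout is a hiding-spot actor for prey and predators, with a construction-sized Hideout box and larger BlockSight box.
; Hideout overlaps track occupants in a map, update their see-through lists, call visibility dispatchers and notify BPC_GetHideout.
; Tick distance-checks occupants against the box's largest extent, printing debug text and firing the hidden event, which snaps BPC_GetHideout owners to the centre.
; CanWelcome compares occupancy to capacity, but overlaps never consult it.
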(event OnComponentBeginOverlap(Hideout)
  (params (OverlappedComponent :type Primitive%20Component%20Object%20Reference) (OtherActor :type Actor%20Object%20Reference) (OtherComp :type Primitive%20Component%20Object%20Reference) (OtherBodyIndex :type Integer) (bFromSweep :type Boolean) (SweepResult :type Hit%20Result%20Structure%20%28by%20ref%29))
  ;[0.3171 1 0] Overlap Pour rendre l'actor dedans caché
  (Utilities|IsValid (Actor|GetComponentbyClass OtherActor "/Game/Blueprints/AddOn/Components/BPC_Prey.BPC_Prey_C")
    (:Is%20Valid
      _)
    (:Is%20Not%20Valid
      (Utilities|IsValid (Actor|GetComponentbyClass OtherActor "/Game/Blueprints/AddOn/Components/BPC_Predator.BPC_Predator_C")
        (:Is%20Valid
          _))))
  (CallFunction|AddActorInside OtherActor))

(event OnComponentEndOverlap(Hideout)
  (params (OverlappedComponent :type Primitive%20Component%20Object%20Reference) (OtherActor :type Actor%20Object%20Reference) (OtherComp :type Primitive%20Component%20Object%20Reference) (OtherBodyIndex :type Integer))
  ;[0.3171 1 0] Overlap Pour rendre l'actor dedans caché
  (CallFunction|RemoveActorInside OtherActor))

(event OnComponentBeginOverlap(BlockSight)
  (params (OverlappedComponent :type Primitive%20Component%20Object%20Reference) (OtherActor :type Actor%20Object%20Reference) (OtherComp :type Primitive%20Component%20Object%20Reference) (OtherBodyIndex :type Integer) (bFromSweep :type Boolean) (SweepResult :type Hit%20Result%20Structure%20%28by%20ref%29)))

(event OnComponentEndOverlap(BlockSight)
  (params (OverlappedComponent :type Primitive%20Component%20Object%20Reference) (OtherActor :type Actor%20Object%20Reference) (OtherComp :type Primitive%20Component%20Object%20Reference) (OtherBodyIndex :type Integer)))

(event Custom|OnActorOutHideout
  (params (Target :type Actor%20Object%20Reference))
  (bind _returnvalue (Actor|GetComponentbyClass Target "/Game/Blueprints/AddOn/Components/BPC_Predator.BPC_Predator_C"))
  (bind _returnvalue_2 (Actor|GetComponentbyClass Target "/Game/Blueprints/AddOn/Components/BPC_Prey.BPC_Prey_C"))
  (bind _returnvalue_3 (Actor|GetComponentbyClass Target "/Game/Blueprints/AddOn/Components/BPC_GetHideout.BPC_GetHideout_C"))
  (Utilities|IsValid _returnvalue_2
    (:Is%20Valid
      (Default|RemoveActorstoSeeThrough _returnvalue_2 self))
    (:Is%20Not%20Valid
      _))
  (Utilities|IsValid _returnvalue
    (:Is%20Valid
      (Default|RemoveActorstoSeeThrough _returnvalue self))
    (:Is%20Not%20Valid
      _))
  (Default|CallEDActorBecomeVisible Target)
  (Utilities|IsValid _returnvalue_3
    (:Is%20Valid
      (Default|OnHideoutLeaved _returnvalue_3))))

(event Custom|OnActorInHideout
  (params (Target :type Actor%20Object%20Reference))
  (bind _returnvalue (Actor|GetComponentbyClass Target "/Game/Blueprints/AddOn/Components/BPC_Prey.BPC_Prey_C"))
  (bind _returnvalue_2 (Actor|GetComponentbyClass Target "/Game/Blueprints/AddOn/Components/BPC_GetHideout.BPC_GetHideout_C"))
  (bind _returnvalue_3 (Actor|GetComponentbyClass Target "/Game/Blueprints/AddOn/Components/BPC_Predator.BPC_Predator_C"))
  (Utilities|IsValid _returnvalue
    (:Is%20Valid
      (Default|AddActorstoSeeThrough _returnvalue self))
    (:Is%20Not%20Valid
      _))
  (Utilities|IsValid _returnvalue_3
    (:Is%20Valid
      (Default|AddActorstoSeeThrough _returnvalue_3 self))
    (:Is%20Not%20Valid
      _))
  (Default|CallEDActorBecomeHidden Target)
  (Utilities|IsValid _returnvalue_2
    (:Is%20Valid
      (Default|OnHideoutEnter _returnvalue_2))))

(event Custom|OnActorHiddenInHideout
  (params (Target :type Actor%20Object%20Reference))
  (bind _returnvalue (Actor|GetComponentbyClass Target "/Game/Blueprints/AddOn/Components/BPC_GetHideout.BPC_GetHideout_C"))
  (Utilities|IsValid _returnvalue
    (:Is%20Valid
      (Default|OnHideoutReached _returnvalue)
      (CallFunction|PlaceActoronSelf Target))
    (:Is%20Not%20Valid
      _))
  (Default|CallEDonActorHiddeninHideout))

(event EventBeginPlay
  (Variables|Default|SetDistanceToBeHidden (Math|Vector|GetMaxElement (Variables|/Script/Engine.BoxComponent|GetBoxExtent (Variables|Default|GetHideout)))))

(event EventTick
  (params (DeltaSeconds :type Float%20%28single-precision%29))
  (bind _currentactorinside (Variables|Default|GetCurrentActorInside))
  (bind _keys (Utilities|Map|Keys (Variables|Default|GetCurrentActorInside)))
  (for _array_element _keys
    (if (CallFunction|ActorHidden _array_element)
      (if (.Value (Utilities|Map|Find _currentactorinside _array_element))
        _
        (else
          (Utilities|Map|Add _currentactorinside _array_element (.ReturnValue (Utilities|Map|Find _currentactorinside _array_element)))
          (CallFunction|OnActorHiddeninHideout _array_element)))
      (Development|PrintText (Utilities|Text|FormatText "{z} HIDE {x} " (Utilities|GetDisplayName self) (Utilities|GetDisplayName _array_element)) true true "(R=0.244897,G=1.000000,B=0.000000,A=1.000000)" 0.0)
      (Development|PrintText (Utilities|Text|FormatText "{x} est à {z} / {w}" (Utilities|GetDisplayName _array_element) (Math|Vector|Distance(Vector) (Transformation|GetActorLocation _array_element) (Transformation|GetActorLocation)) (Variables|Default|GetDistanceToBeHidden)) true true "(R=1.000000,G=0.467075,B=0.000000,A=1.000000)" 0.0)
      (else
        (Development|PrintText (Utilities|Text|FormatText "{x} est à {z} / {w}" (Utilities|GetDisplayName _array_element) (Math|Vector|Distance(Vector) (Transformation|GetActorLocation _array_element) (Transformation|GetActorLocation)) (Variables|Default|GetDistanceToBeHidden)) true true "(R=1.000000,G=0.467075,B=0.000000,A=1.000000)" 0.0)))))

(fn ConstructionScript
  (bind _boxextent (Variables|Param|Size|GetBoxExtent))
  (bind _size (Variables|Param|Size|GetSize))
  (bind _hideout (Variables|Default|GetHideout))
  (bind _returnvalue (* _boxextent _size))
  (Components|Box|SetBoxExtent _hideout _returnvalue true)
  (Development|SetHiddeninGame _hideout (Variables|Param|Rendering|GetHiddenInGame) false)
  (Components|Box|SetBoxExtent (Variables|Default|GetBlockSight) (* _returnvalue 1.2) true))

(fn AddActorInside
  (params (CurrentActorInside :type Actor%20Object%20Reference))
  (if (.ReturnValue (Utilities|Map|Find (Variables|Default|GetCurrentActorInside) CurrentActorInside))
    _
    (else
      (Utilities|Map|Add (Variables|Default|GetCurrentActorInside) CurrentActorInside false)
      (CallFunction|OnActorinHideout CurrentActorInside)))
  (return))

(fn RemoveActorInside
  (params (CurrentActorInside :type Actor%20Object%20Reference))
  (if (Utilities|Map|Contains (Variables|Default|GetCurrentActorInside) CurrentActorInside)
    (CallFunction|OnActorOutHideout CurrentActorInside)
    (Utilities|Map|Remove (Variables|Default|GetCurrentActorInside) CurrentActorInside))
  (return))

(fn ActorHidden
  (params (CurrentActorInside :type Actor%20Object%20Reference))
  (return (<= (Math|Vector|Distance(Vector) (Transformation|GetActorLocation CurrentActorInside) (Transformation|GetActorLocation)) (Variables|Default|GetDistanceToBeHidden))))

(fn CanWelcome
  (return (< (Utilities|Map|Length (Variables|Default|GetCurrentActorInside)) (Variables|Param|GetCapacityHideout))))

(fn PlaceActoronSelf
  (params (Target :type Actor%20Object%20Reference))
  (Transformation|SetActorLocation Target (Transformation|GetActorLocation) true false)
  (return))