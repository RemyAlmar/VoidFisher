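; Spline-based flow current that pulls in the player and pushes them along its path, visualized by a configurable Niagara system.
; Each Tick, distance to the closest spline point drives outer attraction and inner speed-boost zones through player interface messages, with one-shot feedback on inner entry.
; Unless one-directional, push direction scales with the spline tangent's dot product against player facing.
; Looping flow audio follows the closest point, pausing out of range.
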(event Custom|Flow
  (bind _player (Variables|Default|GetPlayer))
  (bind _player_2 (Variables|Default|GetPlayer))
  (bind _player_3 (Variables|Default|GetPlayer))
  (if (CallFunction|IsNearFlow _player_3 (Variables|Force|GetDistanceAttractMax))
    (Class|AudioComponent|SetPaused (Variables|Default|GetS_SFX_Flow) false)
    (Transformation|SetWorldLocation (Variables|Default|GetS_SFX_Flow) (CallFunction|GetClosestLocationonSpline (Transformation|GetActorLocation _player_3)) true false)
    (Class|BPIEnvironmentInfluence|IinFlow(Message) _player (CallFunction|GetAttractPower _player) (* (CallFunction|GetDirectiontoApplyonActorbySpline _player) (Variables|Force|GetForceDirectionPower)))
    (if (CallFunction|IsNearFlow _player_2 (Variables|Force|GetDistanceAttractMin))
      (Class|BPIEnvironmentInfluence|IApplyFlowPower(Message) _player_2 (CallFunction|GetDirectiontoApplyonActorbySpline _player_2) (/ (Variables|Speed|GetFlowPowerSpeed) 1e+02))
      (if (Variables|Default|GetLaunchFeedback)
        (Class|BPIEnvironmentInfluence|SetContinuousFeedback(Message) (Variables|Default|GetPlayer))
        (Variables|Default|SetLaunchFeedback false))
      (else
        (Variables|Default|SetLaunchFeedback true)))
    (else
      (Class|AudioComponent|SetPaused (Variables|Default|GetS_SFX_Flow) true)
      (Class|BPIEnvironmentInfluence|IOutFlow(Message) (Variables|Default|GetPlayer)))))

(event EventBeginPlay
  (bind _s_sfx_flow (Variables|Default|GetS_SFX_Flow))
  (CallFunction|NiagaraInitialize)
  ;[1 0.588 0.3325] SFX
  (Audio|Components|Audio|Play _s_sfx_flow 0.0)
  (Class|AudioComponent|SetPaused _s_sfx_flow true)
  ;[0.1653 1 0.5948] Player init
  (Variables|Default|SetPlayer (Game|Player|GetPlayerPawn 0)))

(event EventTick
  (params (DeltaSeconds :type Float%20%28single-precision%29))
  (CallFunction|Flow))

(fn ConstructionScript
  (CallFunction|NiagaraInitialize))

(fn NiagaraInitialize
  (bind _extent (Variables|Bounds|GetExtent))
  (bind _niagara (Variables|Default|GetNiagara))
  ;[0.1979 0 0.006817] AAAAAAAAAAAAAAAAAAAAAAAAAAAAAAAAAAAAAAAAAAAAAAAAAAAAAAAAAAAAAAAAAAAAAAAAAAAAAAAAAAAAAAAAAAAAAAAAAAAAAAAAAAAAAAAAAAAAAAAAAAAAAAAAAAAAAAAAH
  (Components|Box|SetBoxExtent (Variables|Default|GetBox) _extent false)
  (Class|NiagaraComponent|SetSystemFixedBounds _niagara (Class|KismetMathLibrary|MakeBoxwithOrigin (Transformation|GetActorLocation) _extent))
  (Niagara|SetNiagaraVariable(Object) _niagara "Spline" (Variables|Default|GetSpline))
  (|SetColorVariables)
  (|SetForceVariables)
  (|SetForwardVariables)
  (|SetMagnetVariables)
  (|SetGlobalVariables))

(fn GetSplineDirection
  (params (Target :type Actor%20Object%20Reference))
  (bind _spline (Variables|Default|GetSpline))
  (return (Math|Vector|Normalize (Spline|GetTangentatDistanceAlongSpline _spline (Class|SplineComponent|GetDistanceAlongSplineatLocation _spline (Spline|FindLocationClosesttoWorldLocation _spline (Transformation|GetActorLocation Target) "World") "World") "World"))))

(fn GetDirectionTowardSpline
  (params (TargetLocation :type Vector%20%28by%20ref%29))
  (return (Math|Vector|GetUnitDirection(Vector) TargetLocation (CallFunction|GetClosestLocationonSpline TargetLocation))))

(fn GetDistancetoSpline
  (params (TargetLocation :type Vector%20%28by%20ref%29))
  (return (Math|Vector|Distance(Vector) (CallFunction|GetClosestLocationonSpline TargetLocation) TargetLocation)))

(fn IsNearFlow
  (params (TargetActor :type Actor%20Object%20Reference) (DistanceMax :type Float%20%28double-precision%29))
  (return (<= (CallFunction|GetDistancetoSpline (Transformation|GetActorLocation TargetActor)) DistanceMax)))

(fn GetDirectiontoPush
  (params (TargetActor :type Actor%20Object%20Reference))
  (LocalVariables|SetSplineDirection (CallFunction|GetSplineDirection TargetActor))
  (if (Variables|Force|GetIsOneDirection)
    _
    (else
      (LocalVariables|SetCurrentSens (Math|Vector|DotProduct (LocalVariables|GetSplineDirection) (Transformation|GetActorForwardVector TargetActor)))))
  (return (LocalVariables|GetSplineDirection) (LocalVariables|GetCurrentSens)))

(fn GetDirectiontoApplyonActorbySpline
  (params (TargetActor :type Actor%20Object%20Reference))
  (bind (_direction _sens) (CallFunction|GetDirectiontoPush TargetActor))
  (LocalVariables|SetCurrentDirection (* _direction _sens))
  (return (LocalVariables|GetCurrentDirection)))

(fn GetAttractPower
  (params (TargetActor :type Actor%20Object%20Reference))
  (bind _returnvalue (Transformation|GetActorLocation TargetActor))
  (bind _returnvalue_2 (CallFunction|GetDistancetoSpline _returnvalue))
  (if (<= _returnvalue_2 (Variables|Force|GetDistanceAttractMin))
    (LocalVariables|SetAttractPower _returnvalue_2)
    (else
      (LocalVariables|SetAttractPower (* (Math|Float|SafeDivide (Variables|Force|GetDistanceAttractMax) _returnvalue_2) (Variables|Force|GetAttractionStrength)))))
  (return (* (LocalVariables|GetAttractPower) (CallFunction|GetDirectionTowardSpline _returnvalue))))

(fn GetClosestLocationonSpline
  (params (TargetLocation :type Vector%20%28by%20ref%29))
  (bind _spline (Variables|Default|GetSpline))
  (return (Spline|GetLocationatDistanceAlongSpline _spline (Class|SplineComponent|GetDistanceAlongSplineatLocation _spline TargetLocation "World") "World")))

(fn IsSameDirection
  (params (Player :type Actor%20Object%20Reference))
  (return (>= (Math|Vector|DotProduct (CallFunction|GetSplineDirection Player) (Transformation|GetActorForwardVector Player)) 0.0)))