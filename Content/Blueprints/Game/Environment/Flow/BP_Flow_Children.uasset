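; Child flow actor that adds timed on/off toggling to a parent environmental flow built from a Niagara effect and a spline.
; Visible and Invisible switch Niagara visibility and spline query collision, each setting a timer for the other and printing debug text; nothing here calls either initially.
; Tick runs active and deactive countdowns, skipping the parent tick only when the first returns true and the second false.
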(event EventBeginPlay
  (|CallParentFunction))

(event EventTick
  (params (DeltaSeconds :type Float%20%28single-precision%29))
  (if (CallFunction|TimerNeg (Variables|Default|GetActiveCurrentTime) (Variables|Default|GetActiveTimeMax) 1.0 true)
    (if (CallFunction|TimerNeg (Variables|Default|GetDeactiveCurrentTime) (Variables|Default|GetDeactiveTimeMax) 1.0 true)
      (|CallParentFunction 0.0 :!label _label))
    (else
      (goto _label))))

(fn ConstructionScript
  (|CallParentFunction))

(fn Visible
  (Rendering|SetVisibility (Variables|Default|GetNiagara) true false)
  (Collision|SetCollisionEnabled (Variables|Default|GetSpline) "QueryOnly")
  (Utilities|Time|SetTimerbyFunctionName 0 "Invisible" 0.0)
  (Development|PrintString "Visible (BPC_FLOW)" true true "(R=1.000000,G=0.000000,B=0.041492,A=1.000000)" 2e+01))

(fn Invisible
  (Rendering|SetVisibility (Variables|Default|GetNiagara) false false)
  (Collision|SetCollisionEnabled (Variables|Default|GetSpline) "NoCollision")
  (Utilities|Time|SetTimerbyFunctionName 0 "Visible" 0.0)
  (Development|PrintString "Invisible (BPC_FLOW)" true true "(R=1.000000,G=0.000000,B=0.041492,A=1.000000)" 1e+01))