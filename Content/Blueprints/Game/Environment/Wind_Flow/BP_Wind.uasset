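; BP_Wind is a wind volume actor that pushes physics objects along its up vector.
; The Construction Script sizes the Range box from the RangeX/Y/Z values and raises it to start at the actor origin.
; While anything overlaps the box, Tick casts a grid of debug-drawn Visibility traces upward through it.
; Each hit on a simulating component applies MaxForce at the impact point, so force scales with exposed area.
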(event EventTick
  (params (DeltaSeconds :type Float%20%28single-precision%29))
  (if (> (Utilities|Array|Length (Class|PrimitiveComponent|GetOverlappingComponents (Variables|Default|GetRange))) 0)
    ;[1 0.307 0.8549] Fonction mathématique qui tronque une valeur Float en supprimant sa partie décimale sans l'arrondir
    (for _index (range 0 (Math|Float|Truncate (/ (Variables|Default|GetRangeX) (Variables|Default|GetDistanceBetweenForcesLines))))
      (for _index_2 (range 0 (Math|Float|Truncate (/ (Variables|Default|GetRangeY) (Variables|Default|GetDistanceBetweenForcesLines))))
        ;[0.4742 0.5065 1] Met des limites à la position et range du vent
        (bind (_outhit _returnvalue) (Collision|LineTraceByChannel (Math|Transform|TransformLocation (Transformation|GetActorTransform) (Math|Vector|MakeVector (- (* _index_2 (Variables|Default|GetDistanceBetweenForcesLines)) (/ (Variables|Default|GetRangeX) 2.0)) (- (* _index (Variables|Default|GetDistanceBetweenForcesLines)) (/ (Variables|Default|GetRangeY) 2.0)) 0.0)) (Math|Transform|TransformLocation (Transformation|GetActorTransform) (+ (Math|Vector|MakeVector (- (* _index_2 (Variables|Default|GetDistanceBetweenForcesLines)) (/ (Variables|Default|GetRangeX) 2.0)) (- (* _index (Variables|Default|GetDistanceBetweenForcesLines)) (/ (Variables|Default|GetRangeY) 2.0)) 0.0) (Math|Vector|MakeVector 0.0 0.0 (Variables|Default|GetRangeZ)))) "TraceTypeQuery1" true 0 "ForOneFrame"))
        (if _returnvalue
          (if (Physics|IsSimulatingPhysics (.HitComponent (Collision|BreakHitResult _outhit)) "None")
            (Class|PrimitiveComponent|AddForceatLocation (.HitComponent (Collision|BreakHitResult _outhit)) (* (Transformation|GetActorUpVector) (Variables|Default|GetMaxForce)) (.ImpactPoint (Collision|BreakHitResult _outhit)) "None")))))))

(fn ConstructionScript
  (bind _range (Variables|Default|GetRange))
  (Components|Box|SetBoxExtent (Variables|Default|GetRange) (Math|Vector|MakeVector (/ (Variables|Default|GetRangeX) 2.0) (/ (Variables|Default|GetRangeY) 2.0) (/ (Variables|Default|GetRangeZ) 2.0)) true)
  (Transformation|SetRelativeLocation _range (Math|Vector|MakeVector 0.0 0.0 (.z (Variables|/Script/Engine.BoxComponent|GetBoxExtent _range))) false false))