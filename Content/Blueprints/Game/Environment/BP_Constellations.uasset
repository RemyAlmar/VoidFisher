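; BP_Constellations is an environment Blueprint that shows a constellation on a plane and fades it in and out.
; The construction script creates a dynamic material instance and caches its authored Opacity as a multiplier.
; ISetVisibility plays or reverses the OpacityUpdate timeline, which scales that cached opacity on the material.
; It also returns its CreatureType enum as a string, while GetSkeletalMesh is an empty stub.
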(event Custom|VisibilityOff
  (bind _opacity (Timeline|OpacityUpdate Reverse)
    (:Update
      (Rendering|Material|SetScalarParameterValue (Variables|Default|GetMI_Plane) "Opacity" (* (Variables|Default|GetOpacityMultiplier) _opacity) :!class /Script/Engine.MaterialInstanceDynamic))
    (:Finished
      (Rendering|Material|SetScalarParameterValue (Variables|Default|GetMI_Plane) "Opacity" (* (Variables|Default|GetOpacityMultiplier) _opacity) :!class /Script/Engine.MaterialInstanceDynamic))))

(event Custom|VisibilityOn
  (bind _opacity (Timeline|OpacityUpdate Play)
    (:Update
      (Rendering|Material|SetScalarParameterValue (Variables|Default|GetMI_Plane) "Opacity" (* (Variables|Default|GetOpacityMultiplier) _opacity) :!class /Script/Engine.MaterialInstanceDynamic))
    (:Finished
      (Rendering|Material|SetScalarParameterValue (Variables|Default|GetMI_Plane) "Opacity" (* (Variables|Default|GetOpacityMultiplier) _opacity) :!class /Script/Engine.MaterialInstanceDynamic))))

(event EventISetVisibility
  (params (IsVisible :type Boolean))
  (if IsVisible
    (CallFunction|Visibilityon)
    (else
      (CallFunction|VisibilityOff))))

(fn ConstructionScript
  (bind _returnvalue (Rendering|Material|CreateDynamicMaterialInstance (Variables|Default|GetPlane) 0 (Variables|Param|GetMaterial) "None" :!class /Script/Engine.PrimitiveComponent))
  (bind _output_get (Variables|Default|SetMI_Plane _returnvalue))
  (bind _returnvalue_2 (Rendering|Material|GetScalarParameterValue _output_get "Opacity" :!class /Script/Engine.MaterialInstanceDynamic))
  (Variables|Default|SetOpacityMultiplier _returnvalue_2))

(fn GetSkeletalMesh
  (return 0))

(fn IGetCreatureTypeName
  (return (Utilities|String|EnumtoString (Variables|Param|GetCreatureType))))