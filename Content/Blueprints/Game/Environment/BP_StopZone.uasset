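; BP_StopZone is an environment zone that shows a no-entry warning when something overlaps its invisible wall.
; Overlap begin on SM_InvisibleWall1 creates a single UI_NoEnterInZone widget and adds it to the player screen, without filtering the overlapping actor.
; Overlap end removes and clears that widget.
; BeginPlay caches the BP_PlayerRefonte actor and enables tick, though the graphs shown use neither.
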(event OnComponentBeginOverlap(SM_InvisibleWall1)
  (params (OverlappedComponent :type Primitive%20Component%20Object%20Reference) (OtherActor :type Actor%20Object%20Reference) (OtherComp :type Primitive%20Component%20Object%20Reference) (OtherBodyIndex :type Integer) (bFromSweep :type Boolean) (SweepResult :type Hit%20Result%20Structure%20%28by%20ref%29))
  (Variables|Default|GetWidget
    (:then)
    (:else
      (bind _returnvalue (UserInterface|CreateWidget "/Game/Blueprints/Widgets/Tuto/UI_NoEnterInZone.UI_NoEnterInZone_C"))
      (bind _output_get (Variables|Default|SetWidget _returnvalue))
      (UserInterface|Viewport|AddtoPlayerScreen _output_get))))

(event OnComponentEndOverlap(SM_InvisibleWall1)
  (params (OverlappedComponent :type Primitive%20Component%20Object%20Reference) (OtherActor :type Actor%20Object%20Reference) (OtherComp :type Primitive%20Component%20Object%20Reference) (OtherBodyIndex :type Integer))
  (bind _widget (Variables|Default|GetWidget)
    (:then
      (Widget|RemovefromParent _widget)
      (Variables|Default|SetWidget 0))
    (:else)))

(event EventBeginPlay
  (bind _returnvalue (Actor|GetActorOfClass "/Game/Blueprints/Game/Player/Controllers/BP_PlayerRefonte.BP_PlayerRefonte_C"))
  (Variables|Default|SetPlayer _returnvalue)
  (Actor|Tick|SetActorTickEnabled true))

(fn ConstructionScript)