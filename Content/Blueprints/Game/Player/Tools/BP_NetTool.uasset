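; Net tool for the player that catches creatures touching its box collider while the tool is in use.
; Activation toggles the collider's visibility and overlap events.
; Overlaps query catchable actors through message calls, pass their creature data to the owner, then notify them they were caught.
; The Size stat multiplier scales the net mesh, collider (Y/Z only, re-anchored vertically) and aspirator box, whose overlap handler is empty.
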(event Custom|Net_OnComponentBeginOverlap
  (params (OverlappedComponent :type Primitive%20Component%20Object%20Reference) (OtherActor :type Actor%20Object%20Reference) (OtherComp :type Primitive%20Component%20Object%20Reference) (OtherBodyIndex :type Integer) (bFromSweep :type Boolean) (SweepResult :type Hit%20Result%20Structure%20%28by%20ref%29))
  (if (Variables|Default|GetIsUsed)
    (Development|PrintText "ActorOverlap" true true "(R=0.000000,G=0.660000,B=1.000000,A=1.000000)" 5.0)
    (bind _iscatcheable (Class|BPICatcheable|IsCatcheable(Message) OtherActor))
    (if _iscatcheable
      (Audio|PlaySound2D 0 1.0 1.0 0.0 0 0)
      (bind _data (Class|BPICatcheable|GetData(Message) OtherActor))
      (Class|BPIInventory|AddData(Message) (Components|GetOwner) _data)
      (Development|PrintText (Utilities|Text|FormatText "{name} Added  
{type} SizeType 
It weighs {weight} Kg; 
It size {Size} m; 
Quantity {quantity}" (Utilities|String|EnumtoString (.CreatureName (Utilities|Struct|BreakS_CreatureDetailsInstanced _data))) (Utilities|String|EnumtoString (.CreatureSizeType (Utilities|Struct|BreakS_CreatureDetailsInstanced _data))) (.weight (.CreatureStatSettings (Utilities|Struct|BreakS_CreatureDetailsInstanced _data))) (.size (.CreatureStatSettings (Utilities|Struct|BreakS_CreatureDetailsInstanced _data))) (.quantity (.CreatureStatSettings (Utilities|Struct|BreakS_CreatureDetailsInstanced _data)))))
      (Class|BPICatcheable|Catched(Message) OtherActor)
      (else
        (Development|PrintString "Can't Catcheable")))
    (else
      (Development|PrintText "NotUsed" true true "(R=0.000000,G=0.660000,B=1.000000,A=1.000000)" 5.0))))

(event Custom|Aspirator_OnComponentBeginOverlap
  (params (OverlappedComponent :type Primitive%20Component%20Object%20Reference) (OtherActor :type Actor%20Object%20Reference) (OtherComp :type Primitive%20Component%20Object%20Reference) (OtherBodyIndex :type Integer) (bFromSweep :type Boolean) (SweepResult :type Hit%20Result%20Structure%20%28by%20ref%29)))

(event EventEventActiveToolEvent
  (Rendering|SetVisibility (Variables|Collider|GetNetCollider) true true)
  (Variables|/Script/Engine.PrimitiveComponent|SetbGenerateOverlapEvents (Variables|Collider|GetNetCollider) true)
  (|CallParentFunction))

(event EventEventDeactiveToolEvent
  (Rendering|SetVisibility (Variables|Collider|GetNetCollider) false true)
  (Variables|/Script/Engine.PrimitiveComponent|SetbGenerateOverlapEvents (Variables|Collider|GetNetCollider) false)
  (|CallParentFunction))

(event EventInitialize
  (Collision|BindEventtoOnComponentBeginOverlap (Variables|Collider|GetNetCollider) (EventDispatchers|CreateEvent :!event Custom|Net_OnComponentBeginOverlap))
  (Collision|BindEventtoOnComponentBeginOverlap (Variables|Collider|GetAspiratorCenter) (EventDispatchers|CreateEvent :!event Custom|Aspirator_OnComponentBeginOverlap))
  (CallFunction|UpdateNetSize (.Value (Utilities|Map|Find (Variables|Default|GetCurrentStatMultiplierTools) "NewEnumerator0")))
  (|CallParentFunction))

(event EventEventUseToolEvent
  (|CallParentFunction))

(event EventEventUseToolSecondaryModeEvent
  (|CallParentFunction))

(fn UpdateStat
  (params (Selection :type E_StatUpgrade%20Enum :default "NewEnumerator0") (Multiplier :type Float%20%28double-precision%29))
  (switch Utilities|FlowControl|Switch|SwitchonE_StatUpgrade Selection
    (:NewEnumerator0
      (CallFunction|UpdateNetSize Multiplier))))

(fn UpdateNetSize
  (params (NetMultiplierSize :type Float%20%28double-precision%29))
  (bind _basenetsize (Variables|StatsBase|GetBaseNetSize))
  (bind _baseaspiratorsize (Variables|StatsBase|GetBaseAspiratorSize))
  (bind _returnvalue (* NetMultiplierSize _basenetsize))
  (bind _returnvalue_2 (* NetMultiplierSize _baseaspiratorsize))
  (Components|Box|SetBoxExtent (Variables|Collider|GetNetCollider) (Math|Vector|MakeVector (.x (Variables|StatsBase|GetBaseNetSize)) (.y _returnvalue) (.z _returnvalue)) true)
  (CallFunction|UpdateNetTransform (Variables|Collider|GetNetCollider))
  (Transformation|SetRelativeScale3D (Variables|Collider|GetMeshNet) (* (Class|KismetMathLibrary|VectorOne) NetMultiplierSize))
  (Components|Box|SetBoxExtent (Variables|Collider|GetAspiratorCenter) (Math|Vector|MakeVector (.x _returnvalue_2) (.y _returnvalue_2) (.z _returnvalue_2)) true))

(fn UpdateNetTransform
  (params (Target :type Box%20Component%20Object%20Reference))
  (bind _relativelocation (Variables|/Script/Engine.SceneComponent|GetRelativeLocation Target))
  (Transformation|SetRelativeLocation Target (Math|Vector|MakeVector (.x _relativelocation) (.y _relativelocation) (* (.z (Variables|/Script/Engine.BoxComponent|GetBoxExtent Target)) -1.0)) false false))

(fn Initialization
  (params (NetCollider :type Box%20Component%20Object%20Reference) (AspiratorCenter :type Box%20Component%20Object%20Reference) (MeshNet :type Primitive%20Component%20Object%20Reference))
  (Variables|Collider|SetNetCollider NetCollider)
  (Variables|Collider|SetAspiratorCenter AspiratorCenter)
  (Variables|Collider|SetMeshNet MeshNet)
  (return))