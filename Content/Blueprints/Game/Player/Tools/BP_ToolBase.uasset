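; Base Blueprint for player tools, providing shared activate, deactivate, use, secondary-use and level-upgrade events.
; Initialization deactivates the tool, activation events toggle an IsUsed flag, and both use events only print placeholder text naming the owner.
; Upgrading increments the level, reads that level's stat map from a data table row, caches each value and passes it to UpdateStat, an empty hook in this base.
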(event Custom|Event_UpgradeNextLevel_Event
  (bind _currentlevel (Variables|Default|GetCurrentLevel))
  (Math|Integer|IncrementInt _currentlevel
    (:%20%20
      (CallFunction|UpgradeStatbyLevel _currentlevel))))

(event Custom|Initialize
  (CallFunction|EventDeactiveToolEvent))

(event Custom|Event_ActiveTool_Event
  (Variables|Default|SetIsUsed true))

(event Custom|Event_DeactiveTool_Event
  (Variables|Default|SetIsUsed false))

(event Custom|Event_UseTool_Event
  (Development|PrintText (Utilities|Text|FormatText "{name} is Using (Tool)" (Utilities|GetDisplayName (Components|GetOwner))) true true "(R=0.000000,G=0.660000,B=1.000000,A=1.000000)" 5.0))

(event Custom|Event_UseToolSecondaryMode_Event
  (Development|PrintText (Utilities|Text|FormatText "{name} is Secondary Using (Tool)" (Utilities|GetDisplayName (Components|GetOwner))) true true "(R=0.000000,G=0.660000,B=1.000000,A=1.000000)" 5.0))

(fn UpgradeStatbyLevel
  (params (Level :type Integer))
  (bind _s_upgrading (Variables|Default|GetS_Upgrading))
  (bind _returnvalue (Utilities|GetDataTableRow (.datatable _s_upgrading) (.rowname _s_upgrading))
    (:then
      (bind _keys (Utilities|Map|Keys (.statname (Utilities|Array|Get(acopy) (Utilities|Struct|BreakS_ToolLevelSelection _returnvalue) Level))))
      (for _array_element _keys
        (Utilities|Map|Add (Variables|Default|GetCurrentStatTools) _array_element (.Value (Utilities|Map|Find (.statname (Utilities|Array|Get(acopy) (Utilities|Struct|BreakS_ToolLevelSelection _returnvalue) Level)) _array_element)))
        (CallFunction|UpdateStat _array_element (.Value (Utilities|Map|Find (.statname (Utilities|Array|Get(acopy) (Utilities|Struct|BreakS_ToolLevelSelection _returnvalue) Level)) _array_element)))))
    (:RowNotFound
      _))
  (return))

(fn UpdateStat
  (params (Selection :type E_StatUpgrade%20Enum :default "NewEnumerator0") (Multiplier :type Float%20%28double-precision%29)))