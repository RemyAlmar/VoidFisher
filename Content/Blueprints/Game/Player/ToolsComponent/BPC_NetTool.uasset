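; Player net tool component that sucks in and catches creatures while active, with deploy and storage sounds.
; The aspirator box gathers catchable creatures of allowed sizes and enables Tick only while any remain.
; Tick feeds their physics movement component a pull toward the net collider, stronger when closer.
; Net overlap passes creature data to the owner and triggers the catch; tool stats scale both boxes and suction power.
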(event Custom|Net_OnComponentBeginOverlap
  (params (OverlappedComponent :type Primitive%20Component%20Object%20Reference) (OtherActor :type Actor%20Object%20Reference) (OtherComp :type Primitive%20Component%20Object%20Reference) (OtherBodyIndex :type Integer) (bFromSweep :type Boolean) (SweepResult :type Hit%20Result%20Structure%20%28by%20ref%29))
  ;[0.1232 0.8601 1] Attrape les créatures
  (if (Variables|Default|GetIsActivated)
    (bind _iscatcheable (Class|BPICatcheable|IIsCatcheable(Message) OtherActor))
    (if _iscatcheable
      (bind _data (Class|BPICatcheable|IGetCreatureData(Message) OtherActor))
      (Class|BPIInventory|AddData(Message) (Components|GetOwner) _data)
      (Class|BPICatcheable|ICatched(Message) OtherActor "/Game/VFX/Niagara/Fish/NS_FishCatch.NS_FishCatch"))))

(event Custom|Aspirator_OnComponentBeginOverlap
  (params (OverlappedComponent :type Primitive%20Component%20Object%20Reference) (OtherActor :type Actor%20Object%20Reference) (OtherComp :type Primitive%20Component%20Object%20Reference) (OtherBodyIndex :type Integer) (bFromSweep :type Boolean) (SweepResult :type Hit%20Result%20Structure%20%28by%20ref%29))
  (bind _aspiredactors (Variables|Action|GetAspiredActors))
  ;[0 1 0.3366] Ajoute les actors a aspirés dans la zone
  (bind _asbp_creature_generic (Utilities|Casting|CastToBP_CreatureGeneric OtherActor))
  (if (Utilities|Array|ContainsItem (Variables|Action|GetCreatureSizeCatcheable) (Default|GetCreatureSize _asbp_creature_generic))
    (bind _iscatcheable (Default|IIsCatcheable _asbp_creature_generic))
    (if _iscatcheable
      (Utilities|Array|Add _aspiredactors OtherActor)
      (CallFunction|EDActiveAspiratorEvent (Utilities|Array|IsNotEmpty _aspiredactors)))))

(event Custom|Aspirator_OnComponentEndOverlap
  (params (OverlappedComponent :type Primitive%20Component%20Object%20Reference) (OtherActor :type Actor%20Object%20Reference) (OtherComp :type Primitive%20Component%20Object%20Reference) (OtherBodyIndex :type Integer))
  (bind _aspiredactors (Variables|Action|GetAspiredActors))
  ;[0 1 0.3366] Ajoute les actors a aspirés dans la zone
  (Utilities|IsValid OtherActor
    (:Is%20Valid
      (if (Utilities|Array|ContainsItem _aspiredactors OtherActor)
        (Utilities|Array|RemoveItem _aspiredactors OtherActor)
        (CallFunction|EDActiveAspiratorEvent (Utilities|Array|IsNotEmpty _aspiredactors))))))

(event Custom|ED_ActiveAspirator_Event
  (params (bEnabled :type Boolean))
  ;[0 1 0.3366] Ajoute les actors a aspirés dans la zone
  (Components|Tick|SetComponentTickEnabled bEnabled))

(event EventEDActiveToolEvent
  ;[1 0.7318 0] Activation du Net
  (Variables|/Script/Engine.PrimitiveComponent|SetbGenerateOverlapEvents (Variables|Collider|GetNetCollider) true)
  (Variables|/Script/Engine.PrimitiveComponent|SetbGenerateOverlapEvents (Variables|Collider|GetAspiratorCenter) true)
  (bind _output_get (Variables|Default|SetUseTool_SFX "/Game/SFX/Sounds/NEW_OGG/Filet/SFX_NetDeploymentV2_Cue.SFX_NetDeploymentV2_Cue"))
  (Audio|SpawnSound2D _output_get 1.0 1.0 0.0 "/Game/SFX/Sounds/NEW_OGG/Filet/SC_NetTool.SC_NetTool")
  (|CallParentFunction))

(event EventEDDeactiveToolEvent
  ;[1 0.7318 0] Activation du Net
  (Variables|/Script/Engine.PrimitiveComponent|SetbGenerateOverlapEvents (Variables|Collider|GetNetCollider) false)
  (Variables|/Script/Engine.PrimitiveComponent|SetbGenerateOverlapEvents (Variables|Collider|GetAspiratorCenter) false)
  (bind _output_get (Variables|Default|SetDesactiveToolNet_SFX "/Game/SFX/Sounds/NEW_OGG/Filet/SFX_NetStorageV2_Cue.SFX_NetStorageV2_Cue"))
  (Audio|SpawnSound2D _output_get 1.0 1.0 0.0 "/Game/SFX/Sounds/NEW_OGG/Filet/SC_NetTool.SC_NetTool")
  (|CallParentFunction))

(event EventTick
  (params (DeltaSeconds :type Float%20%28single-precision%29))
  (bind _aspiredactors (Variables|Action|GetAspiredActors))
  ;[0 1 0.3674] Donne une direction vers laquelle tirer les actors de AspiredActors
  (for _array_element _aspiredactors
    (Utilities|IsValid _array_element
      (:Is%20Valid
        (Utilities|IsValid (Actor|GetComponentbyClass _array_element "/Game/Blueprints/AddOn/Components/BPC_ActorPhysicsMovement.BPC_ActorPhysicsMovement_C")
          (:Is%20Valid
            (Default|SetOtherForcesMovement (Actor|GetComponentbyClass _array_element "/Game/Blueprints/AddOn/Components/BPC_ActorPhysicsMovement.BPC_ActorPhysicsMovement_C") (Update|GiveAspirationForce _array_element (Variables|Collider|GetNetCollider))))
          (:Is%20Not%20Valid
            (Utilities|Array|RemoveItem _aspiredactors _array_element :!label _label))))
      (:Is%20Not%20Valid
        (goto _label)))))

(event EventInitialize
  (bind _aspiratorcenter (Variables|Collider|GetAspiratorCenter))
  (Collision|BindEventtoOnComponentBeginOverlap (Variables|Collider|GetNetCollider) (EventDispatchers|CreateEvent :!event Custom|Net_OnComponentBeginOverlap))
  (Collision|BindEventtoOnComponentBeginOverlap _aspiratorcenter (EventDispatchers|CreateEvent :!event Custom|Aspirator_OnComponentBeginOverlap))
  (Collision|AssignOnComponentEndOverlap _aspiratorcenter (EventDispatchers|CreateEvent :!event Custom|Aspirator_OnComponentEndOverlap))
  (|CallParentFunction))

(event EventEDUseToolEvent
  ;[1 0.7318 0] Activation du Net
  (|CallParentFunction))

(event EventEDHoldToolEvent
  (params (DeltaTime :type Float%20%28double-precision%29))
  ;[1 0.7318 0] Activation du Net
  (|CallParentFunction 0.0))

(fn UpdateNetTransform
  (params (Target :type Box%20Component%20Object%20Reference))
  (bind _relativelocation (Variables|/Script/Engine.SceneComponent|GetRelativeLocation Target))
  (Transformation|SetRelativeLocation Target (Math|Vector|MakeVector (.x _relativelocation) (.y _relativelocation) (+ (Variables|NetLocation|GetRelativeLocationZ) (* (.z (Variables|/Script/Engine.BoxComponent|GetBoxExtent Target)) -1.0))) false false))

(fn Initialization
  (params (NetCollider :type Box%20Component%20Object%20Reference) (AspiratorCenter :type Box%20Component%20Object%20Reference) (MeshNet :type Skeletal%20Mesh%20Component%20Object%20Reference))
  (Variables|Collider|SetNetCollider NetCollider)
  (Variables|Collider|SetAspiratorCenter AspiratorCenter)
  (Variables|Collider|SetMeshNet MeshNet)
  (CallFunction|Initialize)
  (return))

(fn GiveAspirationForce
  (params (Target :type Actor%20Object%20Reference) (ActorDirection :type Scene%20Component%20Object%20Reference))
  (bind _returnvalue (Transformation|GetWorldLocation ActorDirection))
  (bind _returnvalue_2 (Transformation|GetActorLocation Target))
  (return (* (Math|Vector|GetUnitDirection(Vector) _returnvalue_2 _returnvalue) (* (/ (Class|KismetMathLibrary|GetMinElement (Variables|/Script/Engine.BoxComponent|GetBoxExtent (Variables|Collider|GetAspiratorCenter))) (Math|Vector|Distance(Vector) _returnvalue_2 _returnvalue)) (* (Variables|StatsBase|GetBaseAspirationPower) (.Value (Utilities|Map|Find (Variables|Default|GetCurrentStatMultiplierTools) "NewEnumerator1")))))))

(fn UpdateAspiratorTransform
  (params (Target :type Box%20Component%20Object%20Reference))
  (Transformation|SetRelativeLocation Target (Math|Vector|MakeVector (/ (.x (Variables|/Script/Engine.BoxComponent|GetBoxExtent Target)) (Variables|NetLocation|GetLocationX)) 0.0 0.0) false false))

(fn UpdateSize
  (bind _currentstattools (Variables|Default|GetCurrentStatTools))
  (bind _aspiratorcenter (Variables|Collider|GetAspiratorCenter))
  (bind _basenetsize (Variables|StatsBase|GetBaseNetSize))
  (bind _value (Utilities|Map|Find _currentstattools "NewEnumerator0"))
  (bind _returnvalue (* _value _basenetsize))
  (Components|Box|SetBoxExtent (Variables|Collider|GetNetCollider) (Math|Vector|MakeVector (.x (Variables|StatsBase|GetBaseNetSize)) (.y _returnvalue) (.z _returnvalue)) true)
  (Update|Transform|UpdateNetTransform (Variables|Collider|GetNetCollider))
  (Components|Box|SetBoxExtent _aspiratorcenter (* (* (Variables|StatsBase|GetBaseNetSize) (Variables|StatsBase|GetBaseAspiratorSizeMultiplier)) _value) true)
  (Update|Transform|UpdateAspiratorTransform _aspiratorcenter)
  (|CallParentFunction))