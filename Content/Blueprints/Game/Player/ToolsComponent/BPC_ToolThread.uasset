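; Tool component that fires a rope-tethered projectile, such as a grappling hook, from a launcher and reels it back.
; It spawns one reusable projectile, linking it to the owner with a cable and physics constraint.
; Tick shortens the constraint as slack appears on an anchored target and reports constraint force as tension.
; On store or a missed target, it retracts the cable, then smoothly realigns and snaps the projectile onto the launcher.
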(event Custom|AttachProjectile
  ;[0.07855 1 0.2737] Replacement du projectile sur le lanceur
  (if (not (Variables|Default|GetHaveToReplacePerfectly))
    (CallFunction|StopPhysicsActor (Variables|ObjecttoSpawn|GetObject))
    (Class|PhysicsConstraintComponent|BreakConstraint (Variables|RopePhysics|GetPhysicsConstraint))
    (Projectile|AttachProjectiletoLauncher)
    (Variables|Default|SetHaveToReplacePerfectly true)))

(event Custom|ReplaceProjectile
  (bind _object (Variables|ObjecttoSpawn|GetObject))
  ;[0.07855 1 0.2737] Replacement du projectile sur le lanceur
  (bind _locaandrotatedone (Projectile|AlignSmoothProjectilewithLauncher))
  (if _locaandrotatedone
    (Transformation|SetActorTransform _object (Math|Transform|MakeTransform (CallFunction|GetProjectileAttachLocation) (Transformation|GetWorldRotation (Variables|SpawnTransform|GetLaunchTransform)) (Transformation|GetActorScale3D _object)))
    (Variables|Default|SetIsStored _locaandrotatedone)
    (CallFunction|SetBringBack (not _locaandrotatedone))
    (Variables|Default|SetHaveToReplacePerfectly (not _locaandrotatedone))
    (Default|SetLaunched (Variables|ObjecttoSpawn|GetObject) false)
    (Audio|Components|Audio|Stop (Variables|Sound|GetSFX_SuckerRetract))
    (Audio|PlaySound2D "/Game/SFX/Sounds/NEW_OGG/Ventouse/SFX_SuckerStorage_Cue.SFX_SuckerStorage_Cue" 1.0 1.0 0.0 0 0)))

(event Custom|Projectile_ED_OnTargetMissing_Event
  ;[1 0.4 0.01108] Projectile Event
  (CallFunction|EDStarttoBringBackEvent))

(event Custom|Projectile_ED_OnActiveProjectileEffect
  ;[1 0.4 0.01108] Projectile Event
)

(event Custom|Projectile_ED_OnActiveSecondaryProjectileEffect
  ;[1 0.4 0.01108] Projectile Event
)

(event Custom|Projectile_ED_OnTargetReached_Event
  ;[1 0.4 0.01108] Projectile Event
  (bind _output_get (Variables|/Script/CableComponent.CableComponent|SetCableLength (Variables|RopePhysics|GetRope) (CallFunction|GetConstrainedComponentDistance)))
  (CallFunction|SetLengthConstraint (Variables|RopePhysics|GetPhysicsConstraint) _output_get))

(event Custom|ED_ApplyTension_Event
  (params (TensionStrength :type Float%20%28double-precision%29) (TensionDirection :type Vector))
  (bind _object (Variables|ObjecttoSpawn|GetObject))
  (bind _returnvalue (Actor|GetComponentbyClass _object "/Game/Blueprints/AddOn/Components/BPC_GrapplingHook.BPC_GrapplingHook_C"))
  ;[1 0.8712 0] Event de l'Utilisation de l'outil
  (Utilities|IsValid _returnvalue
    (:Is%20Valid
      (Default|SetPullStrength _returnvalue TensionStrength TensionDirection))
    (:Is%20Not%20Valid
      _))
  (Default|CallEDApplyTension TensionStrength TensionDirection))

(event Custom|ED_StartToBringBack_Event
  ;[0 1 0.01469] Change la facon de ramener le projectile sur le lanceur
  (CallFunction|SetBringBack true)
  (Default|EDonStartBringBackEvent (Variables|ObjecttoSpawn|GetObject))
  (Default|CallEDStarttoBringBack))

(event Custom|Projectile_GrapHook_ED_OnAnchorPhysicsChanged_Event
  (params (IsPhysics :type Boolean))
  ;[1 0.4 0.01108] Projectile Event
  (Utilities|FlowControl|DelayUntilNextTick)
  (Projectile|AttachRopetoProjectile)
  (CallFunction|ProjectileEDonTargetReachedEvent))

(event Custom|ED_StartTension_Event
  (Default|CallEDStartTension))

(event Custom|ED_EndTension_Event
  (Default|CallEDEndTension))

(event EventEDStoreToolEvent
  ;[0 1 0.01469] Change la facon de ramener le projectile sur le lanceur
  (if (Variables|Default|GetIsStored)
    (if (Variables|Default|GetBringBackCable)
      (CallFunction|AttachProjectile :!label _label)
      (|CallParentFunction :!label _label_2))
    (elif (CallFunction|CanReplaceProjectile)
      (goto _label)
      (else
        (CallFunction|EDStarttoBringBackEvent)
        (goto _label_2)))))

(event EventEDActiveToolEvent
  ;[1 0.8712 0] Event de l'Utilisation de l'outil
  (|CallParentFunction)
  (CallFunction|EDUseToolEvent))

(event EventTick
  (params (DeltaSeconds :type Float%20%28single-precision%29))
  (bind (_tensionstrength _tensiondirection _returnvalue) (CallFunction|HasCableTension))
  ;[0.004252 1 0] Ajustement de la longueur du cable et de la contrainte
  (if (not (Variables|Default|GetIsStored))
    (if (Variables|Default|GetBringBackCable)
      (bind _output_get (Variables|RopePhysics|SetCurrentLength (Math|Interpolation|FInterptoConstant (Variables|RopePhysics|GetCurrentLength) 0.0 (Utilities|Time|GetWorldDeltaSeconds) (Variables|InterpolationSpeed|GetInterpSpeedBringBackRope))))
      (Variables|/Script/CableComponent.CableComponent|SetCableLength (Variables|RopePhysics|GetRope) _output_get)
      (if (<= (Variables|RopePhysics|GetCurrentLength) (CallFunction|GetConstrainedComponentDistance)) ; Si cable tendu grosso modo
        (CallFunction|SetLengthConstraint (Variables|RopePhysics|GetPhysicsConstraint) (Variables|RopePhysics|GetCurrentLength))
        (if (CallFunction|CanReplaceProjectile)
          (CallFunction|AttachProjectile))
        (if (Variables|Default|GetHaveToReplacePerfectly)
          (CallFunction|ReplaceProjectile)))
      (else
        (CallFunction|SetBringBack (CallFunction|ProjectileHasNotReachedTarget))
        (if (Variables|/Game/Blueprints/Game/Player/Spawnables/BP_Projectile.BP_Projectile_C|GetTargetReached (Variables|ObjecttoSpawn|GetObject))
          (bind _output_get_2 (Variables|RopePhysics|SetCurrentLength (CallFunction|DecreaseLengthCablebyDistance)))
          (CallFunction|SetCableLengthLimit _output_get_2)
          (CallFunction|SetIsinTension _returnvalue)
          (if _returnvalue
            (CallFunction|EDApplyTensionEvent _tensionstrength _tensiondirection))
          (else
            (Variables|RopePhysics|SetCurrentLength (CallFunction|GetMaxCurrentLength))))))))

(event EventInitialize
  (bind _projectile (Projectile|CreateProjectile))
  (Variables|ObjecttoSpawn|SetObject _projectile)
  (Projectile|AttachRopetoProjectile)
  (CallFunction|AttachProjectile)
  (Variables|Default|SetHaveToReplacePerfectly false)
  (EventDispatchers|BindEventtoEDActiveProjectileEffect (Variables|ObjecttoSpawn|GetObject) (EventDispatchers|CreateEvent :!event Custom|Projectile_ED_OnActiveProjectileEffect))
  (EventDispatchers|BindEventtoEDSecondaryActionProjectile (Variables|ObjecttoSpawn|GetObject) (EventDispatchers|CreateEvent :!event Custom|Projectile_ED_OnActiveSecondaryProjectileEffect))
  (EventDispatchers|BindEventtoEDonTargetReached (Variables|ObjecttoSpawn|GetObject) (EventDispatchers|CreateEvent :!event Custom|Projectile_ED_OnTargetReached_Event))
  (EventDispatchers|AssignEDonTargetMissing (Variables|ObjecttoSpawn|GetObject) (EventDispatchers|CreateEvent :!event Custom|Projectile_ED_OnTargetMissing_Event))
  (|CallParentFunction)
  (EventDispatchers|BindEventtoEDonAnchorPhysicsChanged (Actor|GetComponentbyClass (Variables|ObjecttoSpawn|GetObject) "/Game/Blueprints/AddOn/Components/BPC_GrapplingHook.BPC_GrapplingHook_C") (EventDispatchers|CreateEvent :!event Custom|Projectile_GrapHook_ED_OnAnchorPhysicsChanged_Event)))

(event EventEDUseToolEvent
  ;[1 0.8712 0] Event de l'Utilisation de l'outil
  (if (Variables|Default|GetIsStored)
    (Variables|Default|SetIsStored false)
    (Variables|Default|SetBringBackCable false)
    (Projectile|AttachRopetoProjectile)
    (CallFunction|SetLengthConstraint (Variables|RopePhysics|GetPhysicsConstraint) (.Value (Utilities|Map|Find (Variables|Default|GetCurrentStatTools) "NewEnumerator0")))
    (Transformation|DetachFromActor (Variables|ObjecttoSpawn|GetObject) "KeepWorld" "KeepWorld" "KeepWorld")
    (Projectile|LaunchProjectile (Math|Vector|GetForwardVector (Variables|SpawnTransform|GetLaunchTransform)))
    (else
      (CallFunction|AttachProjectile)
      (CallFunction|EDStoreToolEvent)))
  (|CallParentFunction))

(fn CreateProjectile
  (bind _currentstatmultipliertools (Variables|Default|GetCurrentStatMultiplierTools))
  (bind _launchtransform (Variables|SpawnTransform|GetLaunchTransform))
  (bind _returnvalue (Transformation|GetWorldTransform _launchtransform))
  (bind (_location _rotation _scale) (Math|Transform|BreakTransform _returnvalue))
  (bind _returnvalue_2 (Game|SpawnActorfromClass (Variables|ObjectToSpawn|GetObjectToSpawn) _returnvalue "Undefined" "MultiplyWithRoot" 0 false false 0))
  (bind _output_get (Variables|ObjecttoSpawn|SetObject _returnvalue_2))
  (Transformation|SetActorTransform _output_get (Math|Transform|MakeTransform (CallFunction|GetProjectileAttachLocation) _rotation _scale))
  (Projectile|AttachProjectiletoLauncher)
  (Default|Initialize (Variables|ObjecttoSpawn|GetObject) (.Value (Utilities|Map|Find _currentstatmultipliertools "NewEnumerator0")) (.Value (Utilities|Map|Find _currentstatmultipliertools "NewEnumerator1")) 15.0 15.0 self)
  (return (Variables|ObjecttoSpawn|GetObject)))

(fn LaunchProjectile
  (params (Direction :type Vector))
  (bind _object (Variables|ObjecttoSpawn|GetObject))
  (CallFunction|LaunchActor _object Direction (.Value (Utilities|Map|Find (Variables|Default|GetCurrentStatTools) "NewEnumerator2")) (CallFunction|GetVelocity (Variables|RopePhysics|GetActorParentRootAttach)))
  (Default|SetLaunched _object true)
  (return))

(fn AttachProjectiletoLauncher
  (Transformation|AttachComponentToComponent (Variables|ObjecttoSpawn|GetObject) (Variables|SpawnTransform|GetLaunchTransform) "None" "KeepWorld" "KeepWorld" "KeepWorld" false)
  (return))

(fn AlignSmoothProjectilewithLauncher
  (bind _interpspeedreplaceprojectile (Variables|InterpolationSpeed|GetInterpSpeedReplaceProjectile))
  (bind _object (Variables|ObjecttoSpawn|GetObject))
  (bind _limittosnapprojectile (Variables|InterpolationSpeed|GetLimitToSnapProjectile))
  (bind _returnvalue (Transformation|GetActorTransform _object))
  (bind _returnvalue_2 (CallFunction|AlignSmooth (Math|Conversions|ToQuaternion(Rotator) (.rotation _returnvalue)) (Math|Conversions|ToQuaternion(Rotator) (Transformation|GetWorldRotation (Variables|SpawnTransform|GetLaunchTransform))) _interpspeedreplaceprojectile))
  (Transformation|SetActorTransform _object (Math|Transform|MakeTransform (CallFunction|SetLocationLerp (.location _returnvalue) (CallFunction|GetProjectileAttachLocation) _interpspeedreplaceprojectile) _returnvalue_2 (.scale _returnvalue)))
  (return (and (Utilities|Operators|EqualEqual (Transformation|GetActorRotation (Variables|ObjecttoSpawn|GetObject)) (Transformation|GetWorldRotation (Variables|SpawnTransform|GetLaunchTransform)) _limittosnapprojectile) (Utilities|Operators|EqualEqual (CallFunction|GetProjectileAttachLocation) (Transformation|GetActorLocation (Variables|ObjecttoSpawn|GetObject)) _limittosnapprojectile))))

(fn AttachRopetoProjectile
  (bind _physicsconstraint (Variables|RopePhysics|GetPhysicsConstraint))
  (bind _object (Variables|ObjecttoSpawn|GetObject))
  (Class|CableComponent|SetAttachEndtoComponent (Variables|RopePhysics|GetRope) (Variables|/Game/Blueprints/Game/Player/Spawnables/BP_Projectile.BP_Projectile_C|GetTransformToAttach _object) "None")
  (Class|PhysicsConstraintComponent|SetConstrainedComponents (Variables|RopePhysics|GetPhysicsConstraint) (Variables|RopePhysics|GetActorParentRootAttach) "None" (Variables|/Game/Blueprints/Game/Player/Spawnables/BP_Projectile.BP_Projectile_C|GetRootCollider _object) "None")
  (Class|PhysicsConstraintComponent|SetConstraintReferencePosition _physicsconstraint "Frame1" (Variables|/Script/Engine.SceneComponent|GetRelativeLocation (Variables|RopePhysics|GetConstraint%20Root)))
  (Class|PhysicsConstraintComponent|SetConstraintReferencePosition _physicsconstraint "Frame2" (Variables|/Script/Engine.SceneComponent|GetRelativeLocation (Variables|/Game/Blueprints/Game/Player/Spawnables/BP_Projectile.BP_Projectile_C|GetTransformToAttach (Variables|ObjecttoSpawn|GetObject))))
  (return))

(fn Initialization
  (params (ParentLaunchTransform :type Scene%20Component%20Object%20Reference) (Rope :type Cable%20Component%20Object%20Reference) (PhysicsConstraint :type Physics%20Constraint%20Component%20Object%20Reference) (ParentAttach :type Primitive%20Component%20Object%20Reference) (BaseStatTools :type Map%20of%20E_StatUpgrade%20Enums%20to%20Reals :default "NewEnumerator0") (ConstraintRoot :type Scene%20Component%20Object%20Reference))
  (Variables|SpawnTransform|SetLaunchTransform ParentLaunchTransform)
  (Variables|RopePhysics|SetRope Rope)
  (Variables|RopePhysics|SetPhysicsConstraint PhysicsConstraint)
  (Variables|RopePhysics|SetActorParentRootAttach ParentAttach)
  (Variables|Default|SetBaseStatTools BaseStatTools)
  (Variables|RopePhysics|SetConstraint%20Root ConstraintRoot))

(fn GetMaxCurrentLength
  (return (Math|Float|Clamp(Float) (CallFunction|GetConstrainedComponentDistance) (Variables|RopePhysics|GetCurrentLength) (.Value (Utilities|Map|Find (Variables|Default|GetCurrentStatTools) "NewEnumerator0")))))

(fn GetConstrainedComponentDistance
  (bind (_outcomponent1 _outbonename1 _outcomponent2) (Class|PhysicsConstraintComponent|GetConstrainedComponents (Variables|RopePhysics|GetPhysicsConstraint)))
  (return (Math|Vector|Distance(Vector) (Transformation|GetWorldLocation _outcomponent1) (Transformation|GetWorldLocation _outcomponent2))))

(fn CanReplaceProjectile
  (return (<= (Variables|RopePhysics|GetCurrentLength) 0.0)))

(fn GetProjectileAttachLocation
  (bind _object (Variables|ObjecttoSpawn|GetObject))
  (return (- (Transformation|GetWorldLocation (Variables|SpawnTransform|GetLaunchTransform)) (- (Transformation|GetWorldLocation (Variables|/Game/Blueprints/Game/Player/Spawnables/BP_Projectile.BP_Projectile_C|GetTransformToAttach _object)) (Transformation|GetWorldLocation (Variables|/Game/Blueprints/Game/Player/Spawnables/BP_Projectile.BP_Projectile_C|GetRootCollider _object))))))

(fn UpdateStats
  (|CallParentFunction)
  (Variables|InterpolationSpeed|SetInterpSpeedBringBackRope (.Value (Utilities|Map|Find (Variables|Default|GetCurrentStatTools) "NewEnumerator0"))))

(fn ProjectileHasNotReachedTarget
  (return (and (not (Variables|/Game/Blueprints/Game/Player/Spawnables/BP_Projectile.BP_Projectile_C|GetTargetReached (Variables|ObjecttoSpawn|GetObject))) (>= (Variables|RopePhysics|GetCurrentLength) (- (.Value (Utilities|Map|Find (Variables|Default|GetCurrentStatTools) "NewEnumerator0")) 1e+02)))))

(fn SetCableLengthLimit
  (params (LengthLimit :type Float%20%28single-precision%29))
  (CallFunction|SetLengthConstraint (Variables|RopePhysics|GetPhysicsConstraint) LengthLimit)
  (Variables|/Script/CableComponent.CableComponent|SetCableLength (Variables|RopePhysics|GetRope) LengthLimit))

(fn DecreaseLengthCablebyDistance
  (return (Math|Float|Clamp(Float) (CallFunction|GetConstrainedComponentDistance) 0.0 (Variables|RopePhysics|GetCurrentLength))))

(fn HasCableTension
  (bind _outlinearforce (Class|PhysicsConstraintComponent|GetConstraintForce (Variables|RopePhysics|GetPhysicsConstraint)))
  (return (Math|Vector|VectorLength _outlinearforce) (Math|Vector|Normalize (Math|Vector|NegateVector _outlinearforce)) (> (Math|Vector|VectorLength _outlinearforce) 0.0)))

(fn GetDistanceObjectandParentRoot
  (return (Math|Vector|Distance(Vector) (Transformation|GetWorldLocation (Variables|RopePhysics|GetActorParentRootAttach)) (Transformation|GetActorLocation (Variables|ObjecttoSpawn|GetObject)))))

(fn SetBringBack
  (params (NextValue :type Boolean))
  (LocalVariables|SetPreviousValue (Variables|Default|GetBringBackCable))
  (Variables|Default|SetBringBackCable NextValue)
  (if (!= (Variables|Default|GetBringBackCable) (LocalVariables|GetPreviousValue)) ; On Value Changed
    (if (Variables|Default|GetBringBackCable) ; OnValue Changed &
      (bind _returnvalue (Audio|CreateSound2D "/Game/SFX/Sounds/NEW_OGG/Ventouse/SFX_CableRetract_Cue.SFX_CableRetract_Cue" 0.5 1.0 0.0 0 false false))
      (bind _output_get (Variables|Sound|SetSFX_SuckerRetract _returnvalue))
      (Audio|Components|Audio|Play _output_get 0.0))))

(fn SetIsinTension
  (params (NextValue :type Boolean))
  (LocalVariables|SetPreviousValue (Variables|Default|GetIsInTension))
  (Variables|Default|SetIsInTension NextValue)
  (if (!= (Variables|Default|GetIsInTension) (LocalVariables|GetPreviousValue)) ; On Value Changed
    (if (Variables|Default|GetIsInTension) ; OnValue Changed &
      (CallFunction|EDStartTensionEvent)
      (else
        (CallFunction|EDEndTensionEvent)))))