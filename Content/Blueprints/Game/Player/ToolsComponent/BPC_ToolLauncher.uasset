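; Player tool component that spawns a projectile and launches it, with a secondary action on the last projectile spawned.
; Using the tool spawns the configured class, initializes it with size and power stat multipliers, then launches it along the launch direction with the player's velocity.
; Secondary use forwards to that stored projectile.
; UpdateLauncherPower computes a stat-scaled current power, but launches use the unscaled base power.
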(event EventToolBaseEDUseToolSecondaryMode
  (Default|CallEDSecondaryActionProjectile (Variables|ObjecttoSpawn|GetObject))
  (|CallParentFunction))

(event EventInitialize
  (|CallParentFunction)
  (bind _asbp_player_refonte (Utilities|Casting|CastToBP_PlayerRefonte (Components|GetOwner)))
  (Variables|Default|SetPlayer _asbp_player_refonte))

(event EventToolBaseEDUseTool
  (bind _projectile (CallFunction|CreateProjectile))
  (bind _player (Variables|Default|GetPlayer)
    (:then
      (CallFunction|LaunchActor _projectile (Variables|Default|GetDirectionToLaunch) (Variables|Statistiques|GetBaseLauncherPower) (Transformation|GetVelocity _player))
      (|CallParentFunction))
    (:else)))

(fn CreateProjectile
  (bind _currentstatmultipliertools (Variables|Default|GetCurrentStatMultiplierTools))
  (bind _returnvalue (Game|SpawnActorfromClass (Variables|ObjectToSpawn|GetObjectToSpawn) (Transformation|GetWorldTransform (Variables|SpawnTransform|GetSpawnTransform)) "Undefined" "MultiplyWithRoot" 0 false true 0))
  (bind _output_get (Variables|ObjecttoSpawn|SetObject _returnvalue))
  (Default|Initialize _output_get (.Value (Utilities|Map|Find _currentstatmultipliertools "NewEnumerator0")) (.Value (Utilities|Map|Find _currentstatmultipliertools "NewEnumerator1")) 15.0 15.0)
  (return _output_get))

(fn UpdateLauncherPower
  (Variables|Statistiques|SetCurrentLauncherPower (* (Variables|Statistiques|GetBaseLauncherPower) (.Value (Utilities|Map|Find (Variables|Default|GetCurrentStatMultiplierTools) "NewEnumerator2"))))
  (|CallParentFunction))