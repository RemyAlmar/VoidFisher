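; Base player tool component handling unlock, activation, use with optional cooldown, storing and upgrades, re-broadcasting each event through dispatchers.
; Upgrades read a data table row per level to multiply base stats, set mesh, anim class and material, and call empty size and power hooks.
; Holding accumulates time toward a trigger threshold, firing first and sustained trigger events.
; Tick decays that time when not held and runs the cooldown timer.
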(event Custom|ED_PostUpgrade_Event
  (Default|CallEDonPostUpgrade))

(event Custom|ED_StoreTool_Event
  (Default|CallEDonStoreTool)
  (if (not (Variables|State|GetIsStored))
    (Audio|PlaySound2D (Variables|Sound|GetStoreTool) 1.0 1.0 0.0 0 0)))

(event Custom|ED_UpgradeNextLevel_Event
  (UpgradeStat|UpgradeStatbyLevel (Level|GetNextLevel))
  (Audio|PlaySound2D (Variables|Sound|GetUpgradeTool_SFX) 1.0 1.0 0.0 0 0)
  (Default|CallEDonUpgradeNextLevel)
  (CallFunction|EDPostUpgradeEvent))

(event Custom|ED_OnStopHoldToolTriggered_Event
  ;[0 1 0.04267] HOLD TRIGGERED : Event de maintien de touche
  (Default|CallEDonStopHoldToolTriggered))

(event Custom|ED_OnFirstHoldToolTriggered_Event
  ;[0 1 0.04267] HOLD TRIGGERED : Event de maintien de touche
  (Variables|TriggeredHoldTime|SetCurrentTriggeredSecondsTime 0.0)
  (Default|CallEDonFirstHoldToolTriggered))

(event Custom|ED_OnStopHoldToolWithoutTriggered_Event
  ;[0 1 0.04267] HOLD TRIGGERED : Event de maintien de touche
  (Default|CallEDonStopHoldToolWithoutTriggered))

(event Custom|ED_OnBeginToHold_Event
  ;[0 1 0.04267] HOLD TRIGGERED : Event de maintien de touche
  (Default|CallEDonBegintoHold))

(event Custom|ED_UpdateOnTimeDecreased_Event
  (params (DeltaTime :type Float%20%28double-precision%29))
  ;[0 1 0.04267] HOLD TRIGGERED : Event de maintien de touche
  (Default|CallEDUpdateonTimeDecreased DeltaTime))

(event Custom|ED_OnTimeReachedZero_Event
  ;[0 1 0.04267] HOLD TRIGGERED : Event de maintien de touche
  (Default|CallEDonTimeReachedZero))

(event Custom|ED_UnlockTool_Event
  (Variables|State|SetIsLock false)
  (Audio|PlaySound2D (Variables|Sound|GetUnlockTool_SFX) 1.0 1.0 0.0 0 0)
  (Default|CallEDonUnlockTool))

(event Custom|Initialize)

(event Custom|ED_StopHoldTool_Event
  (params (DeltaTime :type Float%20%28double-precision%29))
  ;[0 1 0.04267] HOLD TRIGGERED : Event de maintien de touche
  (HoldTime|SetIsHold false)
  (Default|CallEDonStopHoldTool DeltaTime)
  (if (>= DeltaTime (Variables|TriggeredHoldTime|GetTriggeredSecondsRequired))
    (CallFunction|EDonStopHoldToolTriggeredEvent)
    (else
      (CallFunction|EDonStopHoldToolWithoutTriggeredEvent))))

(event Custom|ED_OnHoldToolTriggered_Event
  ;[0 1 0.04267] HOLD TRIGGERED : Event de maintien de touche
  (Default|CallEDonHoldToolTriggered))

(event Custom|ED_ActiveTool_Event
  (Variables|State|SetIsActivated true)
  (Components|Tick|SetComponentTickEnabled true)
  (Default|CallEDonActiveTool))

(event Custom|ED_DeactiveTool_Event
  (Variables|State|SetIsActivated false)
  (CallFunction|EDStoreToolEvent)
  (Default|CallEDonDeactiveTool))

(event Custom|ED_UseTool_Event
  (Default|CallEDonUseTool)
  (if (Variables|Cooldown|GetHasCooldown)
    (Variables|Cooldown|SetCanUseTool false)))

(event Custom|ED_HoldTool_Event
  (params (DeltaTime :type Float%20%28double-precision%29))
  ;[0 1 0.04267] HOLD TRIGGERED : Event de maintien de touche
  (HoldTime|SetIsHold true)
  (HoldTime|IncreaseCurrentTriggeredTime DeltaTime)
  (Default|CallEDonHoldTool DeltaTime))

(event EventTick
  (params (DeltaSeconds :type Float%20%28single-precision%29))
  (Utilities|FlowControl|Sequence
    (:then_0
      (if (not (Variables|TriggeredHoldTime|GetIsHold))
        (HoldTime|DecreaseCurrentTriggeredTime DeltaSeconds)))
    (:then_1
      ;[0 1 0.0242] Cooldown
      (if (Variables|Cooldown|GetHasCooldown)
        (if (not (Variables|Cooldown|GetCanUseTool))
          (Variables|Cooldown|SetCanUseTool (CallFunction|TimerPos (Variables|Cooldown|GetCurrentTime) (Variables|Cooldown|GetMaxTimeCooldown) 1.0 true)))))))

(fn UpgradeStatbyLevel
  (params (Level :type Integer))
  (bind _s_upgrading (Variables|Upgrade|GetS_Upgrading))
  (Variables|State|SetCurrentLevel Level)
  (bind _returnvalue (Utilities|GetDataTableRow (.datatable _s_upgrading) (.rowname _s_upgrading))
    (:then
      (bind _keys (Utilities|Map|Keys (.statname (Utilities|Array|Get(acopy) (Utilities|Struct|BreakS_ToolLevelSelection _returnvalue) Level))))
      (for _array_element _keys
        (Utilities|Map|Add (Variables|Upgrade|GetCurrentStatMultiplierTools) _array_element (.Value (Utilities|Map|Find (.statname (Utilities|Array|Get(acopy) (Utilities|Struct|BreakS_ToolLevelSelection _returnvalue) Level)) _array_element)))
        (Update|UpdateCurrentStat _array_element))
      (Update|UpdateStats)
      (Variables|Default|SetSkeletalMesh (.skeletalmesh (Utilities|Array|Get(acopy) (Utilities|Struct|BreakS_ToolLevelSelection _returnvalue) Level)))
      (Variables|Default|SetAnimClass (.bpanimclass (Utilities|Array|Get(acopy) (Utilities|Struct|BreakS_ToolLevelSelection _returnvalue) Level)))
      (Variables|Default|SetMaterial (.material (Utilities|Array|Get(acopy) (Utilities|Struct|BreakS_ToolLevelSelection _returnvalue) Level))))
    (:RowNotFound
      _))
  (return))

(fn UpdateStats
  (Update|Size|UpdateSize)
  (Update|Power|UpdatePower)
  (Update|LauncherPower|UpdateLauncherPower))

(fn UpdateSize)

(fn UpdatePower)

(fn UpdateLauncherPower)

(fn UpdateCurrentStat
  (params (EStat :type E_StatUpgrade%20Enum%20%28by%20ref%29 :default "NewEnumerator0"))
  (Utilities|Map|Add (Variables|Upgrade|Stats|GetCurrentStatTools) EStat (* (.Value (Utilities|Map|Find (Variables|Upgrade|Stats|GetBaseStatTools) EStat)) (.Value (Utilities|Map|Find (Variables|Upgrade|GetCurrentStatMultiplierTools) EStat)))))

(fn GetTotalLevel
  (bind _s_upgrading (Variables|Upgrade|GetS_Upgrading))
  (bind _returnvalue (Utilities|GetDataTableRow (.datatable _s_upgrading) (.rowname _s_upgrading))
    (:then
      (return (Utilities|Array|Length (.Upgrade (Utilities|Struct|BreakS_ToolLevelSelection _returnvalue)))))))

(fn GetData
  (bind _s_upgrading (Variables|Upgrade|GetS_Upgrading))
  (bind _returnvalue (Utilities|GetDataTableRow (.datatable _s_upgrading) (.rowname _s_upgrading))
    (:then
      (return (Utilities|Array|Get(acopy) (.Upgrade (Utilities|Struct|BreakS_ToolLevelSelection _returnvalue)) (Variables|State|GetCurrentLevel))))))

(fn IncreaseCurrentTriggeredTime
  (params (DeltaTime :type Float%20%28double-precision%29))
  (LocalVariables|SetPreviousValue (Variables|TriggeredHoldTime|GetCurrentTriggeredSecondsTime))
  (Variables|TriggeredHoldTime|SetCurrentTriggeredSecondsTime (+ DeltaTime (LocalVariables|GetPreviousValue)))
  (if (>= (Variables|TriggeredHoldTime|GetCurrentTriggeredSecondsTime) (Variables|TriggeredHoldTime|GetTriggeredSecondsRequired))
    (if (< (LocalVariables|GetPreviousValue) (Variables|TriggeredHoldTime|GetTriggeredSecondsRequired))
      (CallFunction|EDonFirstHoldToolTriggeredEvent)
      (else
        (CallFunction|EDonHoldToolTriggeredEvent)))
    (return)))

(fn DecreaseCurrentTriggeredTime
  (params (DeltaTime :type Float%20%28double-precision%29))
  (HoldTime|SetCurrentTriggeredTime (Math|Interpolation|FInterptoConstant (Variables|TriggeredHoldTime|GetCurrentTriggeredSecondsTime) 0.0 DeltaTime (Variables|TriggeredHoldTime|GetSpeedDecreaseHoldTime)))
  (return))

(fn SetIsHold
  (params (IsHold :type Boolean))
  (LocalVariables|SetPreviousValue (Variables|TriggeredHoldTime|GetIsHold))
  (Variables|TriggeredHoldTime|SetIsHold IsHold)
  (if (!= (Variables|TriggeredHoldTime|GetIsHold) (LocalVariables|GetPreviousValue))
    (if (Variables|TriggeredHoldTime|GetIsHold)
      (CallFunction|EDonBegintoHoldEvent))))

(fn GetNormalizedTime
  (return (Math|Float|NormalizetoRange (Variables|TriggeredHoldTime|GetCurrentTriggeredSecondsTime) 0.0 (Variables|TriggeredHoldTime|GetTriggeredSecondsRequired))))

(fn GetInverseNormalize
  (bind _triggeredsecondsrequired (Variables|TriggeredHoldTime|GetTriggeredSecondsRequired))
  (return (Math|Float|NormalizetoRange (- _triggeredsecondsrequired (Variables|TriggeredHoldTime|GetCurrentTriggeredSecondsTime)) 0.0 _triggeredsecondsrequired)))

(fn GetAlphabyCurrentTime
  (params (TimeMax :type Float%20%28double-precision%29))
  (return (Math|Float|Clamp(Float) (Math|Float|NormalizetoRange (Variables|TriggeredHoldTime|GetCurrentTriggeredSecondsTime) 0.0 TimeMax))))

(fn GetInverseAlphabyCurrentTime
  (params (TimeMax :type Float%20%28double-precision%29))
  (return (Math|Float|Clamp(Float) (Math|Float|NormalizetoRange (- TimeMax (Variables|TriggeredHoldTime|GetCurrentTriggeredSecondsTime)) 0.0 TimeMax))))

(fn SetCurrentTriggeredTime
  (params (NewValue :type Float%20%28double-precision%29))
  (LocalVariables|SetPreviousValue (Variables|TriggeredHoldTime|GetCurrentTriggeredSecondsTime))
  (Variables|TriggeredHoldTime|SetCurrentTriggeredSecondsTime NewValue)
  (if (!= (LocalVariables|GetPreviousValue) (Variables|TriggeredHoldTime|GetCurrentTriggeredSecondsTime))
    (if (> (Variables|TriggeredHoldTime|GetCurrentTriggeredSecondsTime) 0.0)
      (CallFunction|EDUpdateonTimeDecreasedEvent NewValue)
      (else
        (CallFunction|EDonTimeReachedZeroEvent)))
    (return)))

(fn CanbeUpgrade
  (return (<= (Level|GetNextLevel) (Level|GetTotalLevel))))

(fn GetNextLevel
  (return (+ (Variables|State|GetCurrentLevel) 1)))