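; Player ship that steers, collects data into an inventory and uses Net and Sucker tools through a tool manager component.
; Look input rotates a physics reference mesh whose velocity follows eased speed, and the actor copies its transform each Tick.
; Speed drives FOV, turn rate and sound, while a spring arm tilts the ship.
; Spline currents pull it in and change speed by travel direction, with Niagara and rumble feedback.
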(event Custom|OnUpgradeToolManager_Event
  (params (CurrentTool :type E_ToolShip%20Enum :default "NewEnumerator3"))
  ;[0 0.536 1 1 50] Event Feedback
)

(event Custom|FeedbackSpeed
  ;[0 0.536 1 1 50] Event Feedback
  (Camera|SetFieldOfView (Variables|Default|GetCameraController) (Math|Float|Lerp (Variables|Camera|GetFOVBase) (Variables|Camera|GetFOVSpeedMax) (Variables|Speed|GetSpeedDirection))))

(event Custom|FeedbackOnHit
  (bind _forcefeedback (Variables|Default|GetForceFeedback))
  ;[0 0.536 1 1 50] Event Feedback
  (Audio|PlaySound2D "/Game/SFX/Sounds/Player/S_SFX_Collision.S_SFX_Collision" 1.0 1.0 0.0 "/Game/SFX/Sounds/Player/SC_Player.SC_Player" self false)
  (Class|ForceFeedbackComponent|SetForceFeedbackEffect _forcefeedback "/Game/Blueprints/AddOn/ForceFeedback/FFE_Hit.FFE_Hit")
  (Audio|Components|Audio|Play _forcefeedback 0.0)
  (Niagara|SpawnSystematLocation "/Game/VFX/Niagara/NS_ShipColision.NS_ShipColision" (Transformation|GetActorLocation)))

(event Custom|FeedBackOnFlow
  (bind _forcefeedback (Variables|Default|GetForceFeedback))
  ;[0 0.536 1 1 50] Event Feedback
  ;;[1 0 0.2077] Flow
  (Class|ForceFeedbackComponent|SetForceFeedbackEffect _forcefeedback "/Game/Blueprints/AddOn/ForceFeedback/FFE_IsInFlow.FFE_IsInFlow")
  (Audio|Components|Audio|Play _forcefeedback 0.0))

(event Custom|FeedbackOnFlowInBackDirection
  (bind _ns_oar (Variables|Default|GetNS_Oar))
  ;[0 0.536 1 1 50] Event Feedback
  ;;[1 0 0.2077] Flow
  (Class|NiagaraComponent|SetAsset _ns_oar "/Game/VFX/Niagara/NS_ShipInFlow.NS_ShipInFlow" true)
  (Niagara|SetNiagaraVariable(Float) _ns_oar "SpawnRate" 2e+02)
  (Class|ForceFeedbackComponent|SetIntensityMultiplier (Variables|Default|GetForceFeedback) 1.0))

(event Custom|FeedbackOnFlowInRightDirection
  (bind _ns_oar (Variables|Default|GetNS_Oar))
  ;[0 0.536 1 1 50] Event Feedback
  ;;[1 0 0.2077] Flow
  (Class|NiagaraComponent|SetAsset _ns_oar "/Game/VFX/Niagara/NS_AccelerationShip.NS_AccelerationShip" true)
  (Niagara|SetNiagaraVariable(Float) _ns_oar "SpawnRate" 2e+02)
  (Class|ForceFeedbackComponent|SetIntensityMultiplier (Variables|Default|GetForceFeedback) 0.5))

(event Custom|OnUseToolManager_Event
  (params (CurrentTool :type E_ToolShip%20Enum :default "NewEnumerator3"))
  ;[0 0.536 1 1 50] Event Feedback
)

(event Custom|OnUseSecondaryToolManager_Event
  (params (CurrentTool :type E_ToolShip%20Enum :default "NewEnumerator3"))
  ;[0 0.536 1 1 50] Event Feedback
)

(event Custom|OnActiveToolManager_Event
  (params (CurrentTool :type E_ToolShip%20Enum :default "NewEnumerator3"))
  ;[0 0.536 1 1 50] Event Feedback
  (switch Utilities|FlowControl|Switch|SwitchonE_ToolShip CurrentTool
    (:NewEnumerator2
      (Variables|Camera|Distance|SetTargetCameraPosition (Variables|Camera|Distance|GetCameraLengthNet)))))

(event Custom|OnDeactiveToolManager_Event
  (params (CurrentTool :type E_ToolShip%20Enum :default "NewEnumerator3"))
  ;[0 0.536 1 1 50] Event Feedback
  (switch Utilities|FlowControl|Switch|SwitchonE_ToolShip CurrentTool
    (:NewEnumerator2
      (Variables|Camera|Distance|SetTargetCameraPosition (Variables|Camera|Distance|GetCameraLengthBase)))))

(event Custom|OnUnlockToolManager_Event
  (params (CurrentTool :type E_ToolShip%20Enum :default "NewEnumerator3"))
  ;[0 0.536 1 1 50] Event Feedback
)

(event EventHorizontalRoll
  (params (AxisValue :type Float%20%28double-precision%29))
  ;[0.4203 0.3757 1] Roll Ship
  (Transformation|AddLocalRotation (Variables|Default|GetPointReferenceMesh) (Math|Rotator|MakeRotator (* AxisValue (Variables|Movement|Roll|GetRollPlayerSpeed)) 0.0 0.0) false false))

(event Collision|EventHit
  (params (MyComp :type Primitive%20Component%20Object%20Reference) (Other :type Actor%20Object%20Reference) (OtherComp :type Primitive%20Component%20Object%20Reference) (bSelfMoved :type Boolean) (HitLocation :type Vector :default "0, 0, 0") (HitNormal :type Vector :default "0, 0, 0") (NormalImpulse :type Vector :default "0, 0, 0") (Hit :type Hit%20Result%20Structure%20%28by%20ref%29))
  ;[1 0.7569 0] When Ship hit something
  (Variables|Speed|SetSpeedDirection (Math|Interpolation|FInterpTo (Variables|Speed|GetSpeedDirection) 0.0 0.5 5e+01)) ; On ralentit la vitesse du vaisseau \njusqu'à 0 (est compensé par la \nréaccelération du vaisseau)
  (CallFunction|FeedbackonHit))

(event EventTick
  (params (DeltaSeconds :type Float%20%28single-precision%29))
  ;[0.9969 1 0.5568] Move Forward
  (Utilities|FlowControl|Sequence
    (:then_0
      (Movement|MoveShipbySpeed) ; Deplacement du vaisseau
      (Camera|ChangeTargetLength (Variables|Camera|Distance|GetTargetCameraPosition))
      (Audio|Components|Audio|SetVolumeMultiplier (Variables|Default|GetSFX_SpeedSound) (Variables|Speed|GetSpeedDirection) :!class /Script/Engine.AudioComponent)
      (CallFunction|FeedbackSpeed))
    (:then_1
      (Movement|Roll|RollShip DeltaSeconds (.x (stale EventCameraLook LookDirection)) (.y (stale EventCameraLook LookDirection))) ; Gère le roll automatique du vaisseau quand le vaisseau doit tourner dans une direction
      (Transformation|SetActorTransform (Transformation|GetWorldTransform (Variables|Default|GetPointReferenceMesh))) ; pansement pour le root qui a perdu ses parents
    )
    (:then_2
      (Variables|Speed|SetSpeedDirection (Math|Interpolation|FInterpTo (Variables|Speed|GetSpeedDirection) 0.0 DeltaSeconds 0.01)) ; le vaisseau ralentit petit à petit si aucun input n'est activé (input qui influe la vitesse)
      (Movement|ChangeCameraSpeedbySpeedShip) ; la caméra est plus rapide lorsque le vaisseau est à l'arrêt et au contraire plus lente quand le vaisseau est rapide
    )
    (:then_3
      (if (<= (Variables|Speed|GetSpeedDirection) 0.1) ; si le vaisseau est a moins de 10% de sa vitesse
        (Variables|Speed|SetShipStop (Math|Interpolation|FInterpTo (Variables|Speed|GetShipStop) 0.0 DeltaSeconds 5.0)) ; le vaisseau s'arrête
        (else
          (Variables|Speed|SetShipStop (Math|Interpolation|FInterpTo (Variables|Speed|GetShipStop) 1.0 DeltaSeconds 1.0)) ; sinon il avance (ship stop : 1 avance / 0 s'arrête
        )))
    (:then_4
      (if (Variables|Curve|GetIsInTheCourant%20!!!)
        (Variables|Curve|SetIsInTheCourant%20!!! false)
        (else
          (Variables|StatBase|SetBaseMultiplierSpeed 1.0))))))

(event EventFlowEnd
  ;[0 0.536 1 1 50] Event Feedback
  ;;[1 0 0.2077] Flow
  (Niagara|SetNiagaraVariable(Float) (Variables|Default|GetNS_Oar) "SpawnRate" 0.0)
  (Audio|Components|Audio|Stop (Variables|Default|GetForceFeedback)))

(event EventUpdateData
  (params (Data :type Map%20of%20E_CreatureType%20Enums%20to%20Structs :default "NewEnumerator4"))
  ;[0.1602 1 0.3842] Transition Data Inventory
  (Default|UpdateData (Variables|Default|GetHUD_Ship) Data))

(event EventFlowStart
  (params (Spline :type Spline%20Component%20Object%20Reference) (BaseSpeed :type Float%20%28double-precision%29) (SlugSpeed :type Float%20%28double-precision%29) (SubsonicSpeed :type Float%20%28double-precision%29) (MagnetStrength :type Float%20%28double-precision%29) (Damping :type Float%20%28double-precision%29))
  ;[1 1 0.5583] Flow Influence
  (Utilities|FlowControl|Sequence
    (:then_0
      (Curve|SpeedinFlowDirection Spline BaseSpeed SlugSpeed SubsonicSpeed))
    (:then_1
      (bind _returnvalue (Curve|AttractPlayertoCurve Spline MagnetStrength Damping))))
  (Physics|SetPhysicsLinearVelocity (Variables|Default|GetPointReferenceMesh) _returnvalue true "None"))

(event EventAddData
  (params (Data :type S%20Creature%20Details%20Instanced%20Structure))
  ;[0.1602 1 0.3842] Transition Data Inventory
  (Default|AddData (Variables|Default|GetBPC_InventoryComponent) Data)
  (Audio|PlaySound2D "/Game/SFX/Sounds/Fish/S_Capture.S_Capture" 1.0 1.0 0.0 0 0))

(event EventBeginPlay
  ;[1 0.5064 0.8696] Play
  (Utilities|FlowControl|Sequence
    (:then_0
      ;;[1 0.4555 0] Initialize les outils (child Actor)
      (Default|Initialize (Variables|Components|GetBP_SuctionTriggerFish) self))
    (:then_1
      ;;[0 1 0.5447] Ajoute les tools au toolship manager
      (Default|AddTool (Variables|Default|GetBPC_ToolShipManager) (Utilities|Enum|LiteralenumE_ToolShip "NewEnumerator2") (Variables|Default|GetBPC_NetTool))
      (Default|AddTool (Variables|Default|GetBPC_ToolShipManager) (Utilities|Enum|LiteralenumE_ToolShip "NewEnumerator0") (Actor|GetComponentbyClass (Variables|Components|GetBP_SuctionTriggerFish) "/Game/Blueprints/Game/Player/ToolsComponent/BPC_ToolBase.BPC_ToolBase_C"))
      (bind _asbp_hud_ship (Utilities|Casting|CastToBP_HUD_Ship (HUD|GetHUD (Game|GetPlayerController 0))))
      (Variables|Default|SetHUD_Ship _asbp_hud_ship)
      (Niagara|SetNiagaraVariable(Float) (Variables|Default|GetNS_Oar) "SpawnRate" 0.0)
      (|BindingToolShipManager))))

(event EventISelectTool
  (params (ToolSelected :type E_ToolShip%20Enum :default "NewEnumerator3"))
  ;[1 0.9883 0] Tools
  (Default|ToggleTool (Variables|Default|GetBPC_ToolShipManager) ToolSelected))

(event EventIUseTool
  ;[1 0.9883 0] Tools
  (Default|UseTool (Variables|Default|GetBPC_ToolShipManager)))

(event EventCameraLook
  (params (LookDirection :type Vector%202D%20Structure))
  (bind _current_rotation_speed (Variables|Movement|GetCurrent%20Rotation%20Speed))
  ;[0.4203 0.3757 1] Set Rotation
  (Transformation|AddLocalRotation (Variables|Default|GetPointReferenceMesh) (Math|Rotator|MakeRotator 0.0 (* (* (.y LookDirection) _current_rotation_speed) -1.0) (* (.x LookDirection) _current_rotation_speed)) false false) ; Fait tourner le routeur qui fera tourner avec du lag la caméra et le vaisseau
)

(event EventIUnlockTool
  (params (ToolToUnlock :type E_ToolShip%20Enum :default "NewEnumerator3"))
  ;[1 0.9883 0] Tools
  (Default|UnlockTool (Variables|Default|GetBPC_ToolShipManager) ToolToUnlock))

(event EventMoveBack
  (params (Value :type Float%20%28double-precision%29))
  ;[0.9969 1 0.5568] Move Forward
  (Variables|Speed|SetSpeedDirection (Math|Interpolation|FInterpTo (Variables|Speed|GetSpeedDirection) 0.0 (Utilities|Time|GetWorldDeltaSeconds) 1.0)) ; Marche pas pour le moment car creer un bug de caméra à cause des double spring arm
)

(event EventMoveForward
  (params (Value :type Float%20%28double-precision%29))
  ;[0.9969 1 0.5568] Move Forward
  (Variables|Speed|SetSpeedDirection (Math|Interpolation|FInterpTo (Variables|Speed|GetSpeedDirection) Value (Utilities|Time|GetWorldDeltaSeconds) 0.6)) ; On lerp la vitesse jusqu'à .6 (multiplication par rapport à la vitesse max)
)

(event EventIUseSecondaryTool
  ;[1 0.9883 0] Tools
  (Default|UseSecondaryTool (Variables|Default|GetBPC_ToolShipManager)))

(fn ConstructionScript
  (Default|Initialization (Variables|Default|GetBPC_NetTool) (Variables|Default|GetNetCollider) (Variables|Default|GetAspiratorCenter) (Variables|Default|GetSM_Net))
  (bind _output_get (Variables|Camera|Distance|SetCameraLengthBase (Variables|/Script/Engine.SpringArmComponent|GetTargetArmLength (Variables|Default|GetSPA_Cam))))
  (Variables|Camera|Distance|SetTargetCameraPosition _output_get)
  (bind _output_get_2 (Variables|Camera|SetFOVBase (Variables|/Script/Engine.CameraComponent|GetFieldOfView (Variables|Default|GetCameraController))))
  (Variables|Camera|SetFOVSpeedMax (* _output_get_2 1.3))
  (bind _asbp_tool_thread_launcher (Utilities|Casting|CastToBP_ToolThreadLauncher (Variables|/Script/Engine.ChildActorComponent|GetChildActor (Variables|Default|GetSuctionTriggerfish))))
  (Variables|Components|SetBP_SuctionTriggerFish _asbp_tool_thread_launcher))

(fn RollShip
  (params (DeltaTime :type Float%20%28single-precision%29) (Right%20Float :type Float%20%28double-precision%29) (Up%20Float :type Float%20%28double-precision%29))
  (if (!= Right%20Float 0.0) ; Si le roll up (haut et bas) est différent de 0 alors
    (if (> (Variables|Speed|GetShipStop) 0.01) ; Si le vaisseau n'a pas une vitesse null (on a forcé l'arrêt du vaisseau avec le ship stop)
      (if (> (Variables|Speed|GetSpeedDirection) 0.0) ; si le vaisseau est en mouvement
        (|PositiveRoll DeltaTime Right%20Float Up%20Float) ; On fait un roll par rapport à la rotation de la camera
        (return)
        (else
          (|NegativeRoll Right%20Float DeltaTime Up%20Float) ; on fait un roll dans l'autre sens
          (return)))
      (else
        (|ResetRotationto0 (Variables|Default|GetSPA_Ship) DeltaTime) ; Remet le Roll du vaisseau à 0 avec un lerp de manière smooth
        (return)))
    (else
      (|ResetRoll (Variables|Default|GetSPA_Ship) DeltaTime) ; Remet le Roll du vaisseau à 0 avec un lerp de manière smooth
      (return))))

(fn MoveShipbySpeed
  (bind _pointreferencemesh (Variables|Default|GetPointReferenceMesh))
  (bind _returnvalue (Physics|GetPhysicsLinearVelocity _pointreferencemesh "None"))
  (Physics|SetPhysicsLinearVelocity _pointreferencemesh (Math|Vector|Lerp(Vector) _returnvalue (* (Transformation|GetActorForwardVector) (* (* (Variables|Speed|GetSpeedDirection) (* (Variables|StatBase|GetBaseMultiplierSpeed) (Variables|Speed|GetSpeedMax))) (Variables|Speed|GetShipStop))) 0.01) false "None"))

(fn Brake
  (CallFunction|DecreaseValueinTime (Variables|Speed|GetSpeedDirection) 0.0 0.0 1.0 0.0 0.0 false)
  (CallFunction|DecreaseValueExp 0.0 1.0 1.0 1.1 0.0))

(fn ChangeCameraSpeedbySpeedShip
  (Variables|Movement|SetCurrent%20Rotation%20Speed (Math|Float|Clamp(Float) (Math|Float|SafeDivide 0.4 (Math|Float|Absolute(Float) (Variables|Speed|GetSpeedDirection))) 1.0 1.5)))

(fn GetSplineDirection
  (params (Spline :type Spline%20Component%20Object%20Reference))
  (return (Math|Vector|Normalize (Spline|GetTangentatDistanceAlongSpline Spline (Class|SplineComponent|GetDistanceAlongSplineatLocation Spline (Spline|FindLocationClosesttoWorldLocation Spline (Transformation|GetActorLocation) "World") "World") "World"))))

(fn SpeedinFlowDirection
  (params (Spline :type Spline%20Component%20Object%20Reference) (Base%20Speed :type Float%20%28double-precision%29) (Slug%20Speed :type Float%20%28double-precision%29) (Huge%20Speed :type Float%20%28double-precision%29))
  (if (Variables|Movement|GetUseSensFlow)
    (bind _direction__normalize_ (Curve|GetSplineDirection Spline)) ; Renvoie la direction Normalized du point le plus proche dans la spline
    (Variables|Curve|SetIsInTheCourant%20!!! true)
    (bind _returnvalue (Physics|GetPhysicsLinearVelocity (Variables|Default|GetPointReferenceMesh) "None"))
    (if (and (> (Math|Vector|DotProduct _direction__normalize_ (Math|Vector|Normalize _returnvalue)) -0.1) (< (Math|Vector|DotProduct _direction__normalize_ (Math|Vector|Normalize _returnvalue)) 0.1)) ; Est perpendiculaire par rapport à la spline
      (Variables|StatBase|SetBaseMultiplierSpeed Base%20Speed)
      (return)
      (elif (> (Math|Vector|DotProduct _direction__normalize_ (Math|Vector|Normalize _returnvalue)) 0.0) ; va dans le bon sens de la spline
        (Variables|StatBase|SetBaseMultiplierSpeed Huge%20Speed :!label _label)
        (CallFunction|FeedbackonFlowinRightDirection)
        (return)
        (elif (< (Math|Vector|DotProduct _direction__normalize_ (Math|Vector|Normalize _returnvalue)) 0.0) ; va dans le sens inverse de la spline
          (Variables|StatBase|SetBaseMultiplierSpeed Slug%20Speed)
          (CallFunction|FeedbackonFlowinBackDirection)
          (return)
          (else
            (Development|PrintString "Il y a une couille dans le pâté, je répète, il y a une couille dans le pâté" true true "(R=20.000000,G=1.864536,B=0.000000,A=1.000000)" 15.0)))))
    (else
      (goto _label))))

(fn AttractPlayertoCurve
  (params (Spline :type Spline%20Component%20Object%20Reference) (Magnet :type Float%20%28double-precision%29) (Damping :type Float%20%28double-precision%29))
  (bind _returnvalue (Transformation|GetActorLocation))
  (bind _returnvalue_2 (Spline|FindLocationClosesttoWorldLocation Spline _returnvalue "World"))
  (return (* (* (Math|Vector|VectorLength (- _returnvalue _returnvalue_2)) (* (Math|Vector|Normalize (- _returnvalue_2 _returnvalue)) (* (Variables|Curve|GetFlowSpeedMultiplier) Magnet))) (Variables|StatBase|GetDamping))))

(fn ChangeTargetLength
  (params (TargetLength :type Float%20%28double-precision%29))
  (bind _spa_cam (Variables|Default|GetSPA_Cam))
  (Variables|/Script/Engine.SpringArmComponent|SetTargetArmLength _spa_cam (Math|Interpolation|FInterpTo (Variables|/Script/Engine.SpringArmComponent|GetTargetArmLength _spa_cam) TargetLength (Utilities|Time|GetWorldDeltaSeconds) (Variables|Camera|Distance|GetInterpSpeedCam)))
  (return))