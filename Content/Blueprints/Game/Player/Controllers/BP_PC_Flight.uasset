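; Player controller for ship flight that routes Enhanced Input to the possessed pawn and the ship HUD.
; BeginPlay adds player and UI mapping contexts and caches the HUD, which handles menu toggles and key presses.
; Interface messages send movement, camera, tool and skill input to the pawn, with look and free-cam axes scaled by toggleable inversion multipliers.
; Hard-wired T and right-thumbstick presses unlock three tools.
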(event Input|EnhancedActionEvents|EnhancedInputActionIA_CameraLook
  (params (ActionValue :type Vector%202D%20Structure) (ElapsedSeconds :type Float%20%28double-precision%29) (TriggeredSeconds :type Float%20%28double-precision%29) (InputAction :type Input%20Action%20Object%20Reference :default "/Game/Blueprints/Game/Player/Controllers/InputsActions/Player_InputActions/IA_CameraLook.IA_CameraLook"))
  ;[1 0.8122 0.9177] Player Controller
  (:Triggered
    (Class|BPIMoveable|SetDirection(Message) (Game|Player|GetPlayerPawn 0) (Axis|ChangeAxisCamera ActionValue) :!label _label))
  (:Completed
    (goto _label)))

(event Input|EnhancedActionEvents|EnhancedInputActionIA_Accelerate
  (params (ActionValue :type Float%20%28double-precision%29) (ElapsedSeconds :type Float%20%28double-precision%29) (TriggeredSeconds :type Float%20%28double-precision%29) (InputAction :type Input%20Action%20Object%20Reference :default "/Game/Blueprints/Game/Player/Controllers/InputsActions/Player_InputActions/IA_Accelerate.IA_Accelerate"))
  (bind _returnvalue (Game|Player|GetPlayerPawn 0))
  ;[1 0.8122 0.9177] Player Controller
  (:Triggered
    (Class|BPIMoveable|MoveForward(Message) _returnvalue ActionValue))
  (:Completed
    (Class|BPIMoveable|MoveForward(Message) _returnvalue ActionValue)
    (Class|BPIMoveable|BegintoStopSpeed(Message) _returnvalue)))

(event Input|EnhancedActionEvents|EnhancedInputActionIA_Back
  (params (ActionValue :type Boolean) (ElapsedSeconds :type Float%20%28double-precision%29) (TriggeredSeconds :type Float%20%28double-precision%29) (InputAction :type Input%20Action%20Object%20Reference :default "/Game/Blueprints/Game/Player/Controllers/InputsActions/UI_InputActions/IA_Back.IA_Back"))
  ;[0 1 0.3688] HUD Controller
  (Default|ToggleWidgetSubmenu (Variables|Default|GetHUD_Ship) "NewEnumerator3" "NewEnumerator5"))

(event Input|EnhancedActionEvents|EnhancedInputActionIA_Start
  (params (ActionValue :type Boolean) (ElapsedSeconds :type Float%20%28double-precision%29) (TriggeredSeconds :type Float%20%28double-precision%29) (InputAction :type Input%20Action%20Object%20Reference :default "/Game/Blueprints/Game/Player/Controllers/InputsActions/UI_InputActions/IA_Start.IA_Start"))
  ;[0 1 0.3688] HUD Controller
  (Default|ToggleWidgetSubmenu (Variables|Default|GetHUD_Ship) "NewEnumerator3" "NewEnumerator3"))

(event Input|EnhancedActionEvents|EnhancedInputActionIA_FreeCam
  (params (ActionValue :type Vector%202D%20Structure) (ElapsedSeconds :type Float%20%28double-precision%29) (TriggeredSeconds :type Float%20%28double-precision%29) (InputAction :type Input%20Action%20Object%20Reference :default "/Game/Blueprints/Game/Player/Controllers/InputsActions/Player_InputActions/IA_FreeCam.IA_FreeCam"))
  (bind _returnvalue (Game|Player|GetPlayerPawn 0))
  ;[1 0.8122 0.9177] Player Controller
  (:Triggered
    (Class|BPIMoveable|FreeCam(Message) _returnvalue (Axis|ChangeAxisFreeCamera ActionValue)))
  (:Completed
    (Class|BPIMoveable|EndFreeCam(Message) _returnvalue)))

(event Input|EnhancedActionEvents|EnhancedInputActionIA_Scroll
  (params (ActionValue :type Float%20%28double-precision%29) (ElapsedSeconds :type Float%20%28double-precision%29) (TriggeredSeconds :type Float%20%28double-precision%29) (InputAction :type Input%20Action%20Object%20Reference :default "/Game/Blueprints/Game/Player/Controllers/InputsActions/UI_InputActions/IA_Scroll.IA_Scroll"))
  ;[0 1 0.3688] HUD Controller
)

(event Input|EnhancedActionEvents|EnhancedInputActionIA_Skill
  (params (ActionValue :type Boolean) (ElapsedSeconds :type Float%20%28double-precision%29) (TriggeredSeconds :type Float%20%28double-precision%29) (InputAction :type Input%20Action%20Object%20Reference :default "/Game/Blueprints/Game/Player/Controllers/InputsActions/Player_InputActions/IA_Skill.IA_Skill"))
  (bind _returnvalue (Game|Player|GetPlayerPawn 0))
  ;[1 0.8122 0.9177] Player Controller
  (:Triggered
    (Class|BPIToolUseable|IUseSkillContinue(Message) _returnvalue))
  (:Started
    (Class|BPIToolUseable|IUseSkillOnce(Message) _returnvalue))
  (:Canceled
    (Class|BPIToolUseable|IUseSkillCanceled(Message) _returnvalue :!label _label))
  (:Completed
    (goto _label)))

(event Input|EnhancedActionEvents|EnhancedInputActionIA_Decelerate
  (params (ActionValue :type Float%20%28double-precision%29) (ElapsedSeconds :type Float%20%28double-precision%29) (TriggeredSeconds :type Float%20%28double-precision%29) (InputAction :type Input%20Action%20Object%20Reference :default "/Game/Blueprints/Game/Player/Controllers/InputsActions/Player_InputActions/IA_Decelerate.IA_Decelerate"))
  (bind _returnvalue (Game|Player|GetPlayerPawn 0))
  ;[1 0.8122 0.9177] Player Controller
  (:Triggered
    (Class|BPIMoveable|MoveBack(Message) _returnvalue ActionValue))
  (:Completed
    (Class|BPIMoveable|MoveBack(Message) _returnvalue ActionValue)
    (Class|BPIMoveable|BegintoStopSpeed(Message) _returnvalue)))

(event Input|EnhancedActionEvents|EnhancedInputActionIA_ActiveSuckerTool
  (params (ActionValue :type Boolean) (ElapsedSeconds :type Float%20%28double-precision%29) (TriggeredSeconds :type Float%20%28double-precision%29) (InputAction :type Input%20Action%20Object%20Reference :default "/Game/Blueprints/Game/Player/Controllers/InputsActions/Player_InputActions/IA_ActiveSuckerTool.IA_ActiveSuckerTool"))
  ;[1 0.8122 0.9177] Player Controller
  (Class|BPIToolUseable|ISelectTool(Message) (Game|Player|GetPlayerPawn 0) "NewEnumerator0"))

(event Input|EnhancedActionEvents|EnhancedInputActionIA_Movement
  (params (ActionValue :type Vector%202D%20Structure) (ElapsedSeconds :type Float%20%28double-precision%29) (TriggeredSeconds :type Float%20%28double-precision%29) (InputAction :type Input%20Action%20Object%20Reference :default "/Game/Blueprints/Game/Player/Controllers/InputsActions/Player_InputActions/IA_Movement.IA_Movement"))
  ;[1 0.8122 0.9177] Player Controller
  (Class|BPIMoveable|Roll(Message) (Game|Player|GetPlayerPawn 0) ActionValue))

(event Input|EnhancedActionEvents|EnhancedInputActionIA_UseSecondaryTool
  (params (ActionValue :type Boolean) (ElapsedSeconds :type Float%20%28double-precision%29) (TriggeredSeconds :type Float%20%28double-precision%29) (InputAction :type Input%20Action%20Object%20Reference :default "/Game/Blueprints/Game/Player/Controllers/InputsActions/Player_InputActions/IA_UseSecondaryTool.IA_UseSecondaryTool"))
  ;[1 0.8122 0.9177] Player Controller
  (Class|BPIToolUseable|IUseSecondaryTool(Message) (Game|Player|GetPlayerPawn 0)))

(event Input|EnhancedActionEvents|EnhancedInputActionIA_ActiveBaitTool
  (params (ActionValue :type Boolean) (ElapsedSeconds :type Float%20%28double-precision%29) (TriggeredSeconds :type Float%20%28double-precision%29) (InputAction :type Input%20Action%20Object%20Reference :default "/Game/Blueprints/Game/Player/Controllers/InputsActions/Player_InputActions/IA_ActiveBaitTool.IA_ActiveBaitTool"))
  ;[1 0.8122 0.9177] Player Controller
  (Class|BPIToolUseable|ISelectTool(Message) (Game|Player|GetPlayerPawn 0) "NewEnumerator1"))

(event Input|EnhancedActionEvents|EnhancedInputActionIA_ActiveNetTool
  (params (ActionValue :type Boolean) (ElapsedSeconds :type Float%20%28double-precision%29) (TriggeredSeconds :type Float%20%28double-precision%29) (InputAction :type Input%20Action%20Object%20Reference :default "/Game/Blueprints/Game/Player/Controllers/InputsActions/Player_InputActions/IA_ActiveNetTool.IA_ActiveNetTool"))
  ;[1 0.8122 0.9177] Player Controller
  (Class|BPIToolUseable|ISelectTool(Message) (Game|Player|GetPlayerPawn 0) "NewEnumerator2"))

(event Input|EnhancedActionEvents|EnhancedInputActionIA_UseTool
  (params (ActionValue :type Boolean) (ElapsedSeconds :type Float%20%28double-precision%29) (TriggeredSeconds :type Float%20%28double-precision%29) (InputAction :type Input%20Action%20Object%20Reference :default "/Game/Blueprints/Game/Player/Controllers/InputsActions/Player_InputActions/IA_UseTool.IA_UseTool"))
  ;[1 0.8122 0.9177] Player Controller
  (Class|BPIToolUseable|IUseTool(Message) (Game|Player|GetPlayerPawn 0)))

(event Input|EnhancedActionEvents|EnhancedInputActionIA_Inventory
  (params (ActionValue :type Boolean) (ElapsedSeconds :type Float%20%28double-precision%29) (TriggeredSeconds :type Float%20%28double-precision%29) (InputAction :type Input%20Action%20Object%20Reference :default "/Game/Blueprints/Game/Player/Controllers/InputsActions/UI_InputActions/IA_Inventory.IA_Inventory"))
  ;[0 1 0.3688] HUD Controller
  (Default|ToggleWidget (Variables|Default|GetHUD_Ship) "NewEnumerator4"))

(event EventBeginPlay
  (bind _returnvalue (Game|GetPlayerController 0))
  (bind _returnvalue_2 (Game|GetPlayerController 0))
  (bind _returnvalue_3 (PlayerController|LocalPlayerSubsystems|GetEnhancedInputLocalPlayerSubsystem _returnvalue_2))
  (bind _returnvalue_4 (PlayerController|LocalPlayerSubsystems|GetEnhancedInputLocalPlayerSubsystem _returnvalue))
  (bind _returnvalue_5 (Class|EnhancedInputSubsystemInterface|GetUserSettings _returnvalue_4))
  (Utilities|FlowControl|Sequence
    (:then_0
      (Utilities|IsValid _returnvalue_4
        (:Is%20Valid
          (Input|AddMappingContext _returnvalue_4 "/Game/Blueprints/Game/Player/Controllers/InputsActions/IMC_Player_Controller.IMC_Player_Controller" 1 "(bIgnoreAllPressedKeysUntilRelease=True,bForceImmediately=False,bNotifyUserSettings=False)")
          (if (not (Class|EnhancedInputUserSettings|IsMappingContextRegistered _returnvalue_5 "/Game/Blueprints/Game/Player/Controllers/InputsActions/IMC_Player_Controller.IMC_Player_Controller"))
            (Class|EnhancedInputUserSettings|RegisterInputMappingContext _returnvalue_5 "/Game/Blueprints/Game/Player/Controllers/InputsActions/IMC_Player_Controller.IMC_Player_Controller")))))
    (:then_1
      (bind _asbp_hud_ship (Utilities|Casting|CastToBP_HUD_Ship (HUD|GetHUD)))
      (Variables|Default|SetHUD_Ship _asbp_hud_ship)
      (Utilities|IsValid _returnvalue_3
        (:Is%20Valid
          (Input|AddMappingContext _returnvalue_3 "/Game/Blueprints/Game/Player/Controllers/InputsActions/IMC_UI_Controller.IMC_UI_Controller" 0 "(bIgnoreAllPressedKeysUntilRelease=True,bForceImmediately=False,bNotifyUserSettings=False)"))))))

(event Input|GamepadEvents|GamepadRightThumbstick
  (params (Key :type Key%20Structure :default "None"))
  ;[1 0.8122 0.9177] Player Controller
  (:Pressed
    (Class|BPIToolUseable|IUnlockTool(Message) (Game|Player|GetPlayerPawn 0) "NewEnumerator2")
    (Class|BPIToolUseable|IUnlockTool(Message) (Game|Player|GetPlayerPawn 0) "NewEnumerator1")
    (Class|BPIToolUseable|IUnlockTool(Message) (Game|Player|GetPlayerPawn 0) "NewEnumerator0")))

(event Input|KeyboardEvents|AnyKey
  (params (Key :type Key%20Structure :default "None"))
  ;[1 0.8122 0.9177] Player Controller
  (:Pressed
    (Default|OnKeyDown (Variables|Default|GetHUD_Ship) Key)
    (Default|CallEDonKey Key)))

(event Input|KeyboardEvents|T
  (params (Key :type Key%20Structure :default "None"))
  ;[1 0.8122 0.9177] Player Controller
  (:Pressed
    (Class|BPIToolUseable|IUnlockTool(Message) (Game|Player|GetPlayerPawn 0) "NewEnumerator2")
    (Class|BPIToolUseable|IUnlockTool(Message) (Game|Player|GetPlayerPawn 0) "NewEnumerator1")
    (Class|BPIToolUseable|IUnlockTool(Message) (Game|Player|GetPlayerPawn 0) "NewEnumerator0")))

(fn ConstructionScript)

(fn InvertCameraAxis
  (params (Camera%20/%20Free%20Camera :type Boolean) (X/Y :type Boolean))
  (if Camera%20/%20Free%20Camera
    ;[1 0.8575 0.6561] Ship Direction
    (if X/Y
      (if (== (Variables|Camera|GetB_Invert_Camera_Axis_X) 1.0)
        (Variables|Camera|SetB_Invert_Camera_Axis_X -1.0)
        (else
          (Variables|Camera|SetB_Invert_Camera_Axis_X 1.0)))
      (return)
      (else
        (if (== (Variables|Camera|GetB_Invert_Camera_Axis_Y) 1.0)
          (Variables|Camera|SetB_Invert_Camera_Axis_Y -1.0)
          (else
            (Variables|Camera|SetB_Invert_Camera_Axis_Y 1.0)))
        (return)))
    (else
      ;[0.9555 0.8509 1] Free Cam
      (if X/Y
        (if (== (Variables|FreeCamera|GetB_Invert_FreeCamera_Axis_X) 1.0)
          (Variables|FreeCamera|SetB_Invert_FreeCamera_Axis_X -1.0)
          (else
            (Variables|FreeCamera|SetB_Invert_FreeCamera_Axis_X 1.0)))
        (return)
        (else
          (if (== (Variables|FreeCamera|GetB_Invert_FreeCamera_Axis_Y) 1.0)
            (Variables|FreeCamera|SetB_Invert_FreeCamera_Axis_Y -1.0)
            (else
              (Variables|FreeCamera|SetB_Invert_FreeCamera_Axis_Y 1.0)))
          (return))))))

(fn ChangeAxisCamera
  (params (2D%20Axe :type Vector%202D%20Structure))
  (return (Math|Vector2D|MakeVector2D (* (.x 2D%20Axe) (Variables|Camera|GetB_Invert_Camera_Axis_X)) (* (.y 2D%20Axe) (Variables|Camera|GetB_Invert_Camera_Axis_Y)))))

(fn ChangeAxisFreeCamera
  (params (2D%20Axe :type Vector%202D%20Structure))
  (return (Math|Vector2D|MakeVector2D (* (.x 2D%20Axe) (Variables|FreeCamera|GetB_Invert_FreeCamera_Axis_X)) (* (.y 2D%20Axe) (Variables|FreeCamera|GetB_Invert_FreeCamera_Axis_Y)))))