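; Player ship that drives physics movement, switches between net, bait and sucker tools, and passes captured creature data to its inventory.
; Throttle input interpolates a current speed, which Tick turns into forward velocity on the main collider, then damps.
; In flow splines, heading dotted with the tangent picks a speed multiplier (stored but unread here) and VFX/rumble feedback, alongside a spring-like pull toward the curve.
; Hit is empty and its collision feedback is disconnected.
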(event Collision|EventHit
  (params (MyComp :type Primitive%20Component%20Object%20Reference) (Other :type Actor%20Object%20Reference) (OtherComp :type Primitive%20Component%20Object%20Reference) (bSelfMoved :type Boolean) (HitLocation :type Vector :default "0, 0, 0") (HitNormal :type Vector :default "0, 0, 0") (NormalImpulse :type Vector :default "0, 0, 0") (Hit :type Hit%20Result%20Structure%20%28by%20ref%29))
  ;[1 0.7569 0] When Ship hit something
)

(event EventFlowEnd
  ;[1 1 0.5583] Flow Influence
  ;;[0.5654 1 0.6811] Feedback
  (|StopFeedBack))

(event EventUpdateData
  (params (Data :type Map%20of%20E_CreatureType%20Enums%20to%20Structs :default "NewEnumerator3"))
  ;[0.1602 1 0.3842] Transition Data Inventory
  (Default|UpdateData (Variables|HUD|GetHUD_Ship) Data))

(event EventFlowStart
  (params (Spline :type Spline%20Component%20Object%20Reference) (BaseSpeed :type Float%20%28double-precision%29) (SlugSpeed :type Float%20%28double-precision%29) (SubsonicSpeed :type Float%20%28double-precision%29) (MagnetStrength :type Float%20%28double-precision%29) (Damping :type Float%20%28double-precision%29))
  (bind _forcefeedback (Variables|Default|GetForceFeedback))
  ;[1 1 0.5583] Flow Influence
  (Utilities|FlowControl|Sequence
    (:then_0
      (bind _pointreferencemesh (Curve|SpeedinFlowDirection Spline BaseSpeed SlugSpeed SubsonicSpeed)))
    (:then_1
      (bind _returnvalue (Curve|AttractPlayertoCurve Spline MagnetStrength Damping))))
  (Physics|SetPhysicsLinearVelocity _pointreferencemesh _returnvalue true "None")
  ;;[0.5654 1 0.6811] Feedback
  (Class|ForceFeedbackComponent|SetForceFeedbackEffect _forcefeedback "/Game/Blueprints/AddOn/ForceFeedback/FFE_IsInFlow.FFE_IsInFlow")
  (Audio|Components|Audio|Play _forcefeedback 0.0))

(event EventMoveForward
  (params (Value :type Float%20%28double-precision%29))
  ;[0 1 0.257] Move
  (Physics|SpeedSystem|IncreaseCurrentSpeed Value))

(event EventAddData
  (params (CreatureType :type E_CreatureType%20Enum :default "NewEnumerator3") (Data :type S%20Catcheable%20Data%20Structure))
  ;[0.1602 1 0.3842] Transition Data Inventory
  (Default|AddData (Variables|Default|GetBP_InventoryComponent) CreatureType Data)
  (Audio|PlaySound2D "/Game/SFX/Sounds/Fish/S_Capture.S_Capture" 1.0 1.0 0.0 0 0))

(event EventTick
  (params (DeltaSeconds :type Float%20%28single-precision%29))
  (Physics|VelocityForce|ApplyForceShipForward)
  (Physics|VelocityForce|ApplyVelocity)
  (Physics|VelocityForce|ApplyDamping)
  (bind _returnvalue (Physics|GetPhysicsLinearVelocity (Variables|Default|GetMainCollider) "None"))
  (Development|PrintText (Utilities|Text|FormatText "Current Velocity : {v}" (Utilities|String|ToString(Vector) _returnvalue)) true true "(R=1.000000,G=0.823312,B=0.000000,A=1.000000)" 0.0))

(event EventMoveBack
  (params (Value :type Float%20%28double-precision%29))
  ;[0 1 0.257] Move
  (Physics|SpeedSystem|DecreaseCurrentSpeed Value))

(event EventBeginPlay
  ;[1 0.5064 0.8696] Play
  (Default|AddTool (Variables|Default|GetBP_ToolShipManager) (Utilities|Enum|LiteralenumE_ToolShip "NewEnumerator2") (Variables|Default|GetBP_NetTool))
  (Default|AddTool (Variables|Default|GetBP_ToolShipManager) (Utilities|Enum|LiteralenumE_ToolShip "NewEnumerator1") (Variables|Default|GetBP_BaitTool))
  (Default|AddTool (Variables|Default|GetBP_ToolShipManager) (Utilities|Enum|LiteralenumE_ToolShip "NewEnumerator0") (Variables|Default|GetBP_SuckerTool))
  (bind _asbp_hud_ship (Utilities|Casting|CastToBP_HUD_Ship (HUD|GetHUD (Game|GetPlayerController 0))))
  (Variables|HUD|SetHUD_Ship _asbp_hud_ship)
  (Niagara|SetNiagaraVariable(Float) (Variables|Default|GetNS_ShipInFlow) "SpawnRate" 0.0))

(event EventISelectTool
  (params (ToolSelected :type E_ToolShip%20Enum :default "NewEnumerator3"))
  ;[1 0.9883 0] Tools
  (Default|ToggleTool (Variables|Default|GetBP_ToolShipManager) ToolSelected))

(event EventIUseTool
  ;[1 0.9883 0] Tools
  (Default|UseTool (Variables|Default|GetBP_ToolShipManager)))

(event EventIUnlockTool
  (params (ToolToUnlock :type E_ToolShip%20Enum :default "NewEnumerator3"))
  ;[1 0.9883 0] Tools
  (Default|UnlockTool (Variables|Default|GetBP_ToolShipManager) ToolToUnlock))

(event EventIUseSecondaryTool
  ;[1 0.9883 0] Tools
  (Default|UseSecondaryTool (Variables|Default|GetBP_ToolShipManager))
  (Audio|PlaySound2D "/Game/SFX/Sounds/Player/S_SortieOutil.S_SortieOutil" 1.0 1.0 0.0 0 0))

(fn ConstructionScript
  (bind _bp_nettool (Variables|Default|GetBP_NetTool))
  (Variables|/Game/Blueprints/Game/Player/Tools/BP_NetTool.BP_NetTool_C|SetNetCollider _bp_nettool (Variables|Default|GetNetCollider))
  (Default|Initialize _bp_nettool)
  (Variables|/Game/Blueprints/Game/Player/Tools/BP_ToolLauncher.BP_ToolLauncher_C|SetSpawnTransform (Variables|Default|GetBP_BaitTool) (Variables|Default|GetBH_Launcher))
  (Variables|/Game/Blueprints/Game/Player/Tools/BP_ToolLauncher.BP_ToolLauncher_C|SetSpawnTransform (Variables|Default|GetBP_SuckerTool) (Variables|Default|GetBH_Launcher)))

(fn AttractPlayertoCurve
  (params (Spline :type Spline%20Component%20Object%20Reference) (Magnet :type Float%20%28double-precision%29) (Damping :type Float%20%28double-precision%29))
  (bind _returnvalue (Transformation|GetActorLocation))
  (bind _returnvalue_2 (Spline|FindLocationClosesttoWorldLocation Spline _returnvalue "World"))
  (return (* Damping (* (* (Math|Vector|Normalize (- _returnvalue_2 _returnvalue)) (* Magnet Damping)) (Math|Vector|VectorLength (- _returnvalue _returnvalue_2))))))

(fn SpeedinFlowDirection
  (params (Spline :type Spline%20Component%20Object%20Reference) (Base%20Speed :type Float%20%28double-precision%29) (Slug%20Speed :type Float%20%28double-precision%29) (Huge%20Speed :type Float%20%28double-precision%29))
  (bind _direction__normalize_ (Curve|GetSplineDirection Spline)) ; Renvoie la direction Normalized du point le plus proche dans la spline
  (Variables|Curve|SetIsInTheCourant%20!!! true)
  (bind _returnvalue (Physics|GetPhysicsLinearVelocity (Variables|Default|GetMainCollider) "None"))
  (if (and (> (Math|Vector|DotProduct (Math|Vector|Normalize _returnvalue) _direction__normalize_) -0.1) (< (Math|Vector|DotProduct (Math|Vector|Normalize _returnvalue) _direction__normalize_) 0.1)) ; Est perpendiculaire par rapport à la spline
    (Variables|Curve|SetFlowSpeedMultiplayer Base%20Speed)
    (elif (> (Math|Vector|DotProduct (Math|Vector|Normalize _returnvalue) _direction__normalize_) 0.0) ; va dans le bon sens de la spline
      (Variables|Curve|SetFlowSpeedMultiplayer Huge%20Speed)
      ;[0.5654 1 0.6811] Feedback
      (|SetFeedBacks)
      (elif (< (Math|Vector|DotProduct (Math|Vector|Normalize _returnvalue) _direction__normalize_) 0.0) ; va dans le sens inverse de la spline
        (Variables|Curve|SetFlowSpeedMultiplayer Slug%20Speed)
        (|SetFeedBack)
        (else
          (Development|PrintString "Il y a une couille dans le pâté, je répète, il y a une couille dans le pâté" true true "(R=20.000000,G=1.864536,B=0.000000,A=1.000000)" 15.0)))))
  (return 0))

(fn GetSplineDirection
  (params (Spline :type Spline%20Component%20Object%20Reference))
  (return (Math|Vector|Normalize (Spline|GetTangentatDistanceAlongSpline Spline (Class|SplineComponent|GetDistanceAlongSplineatLocation Spline (Spline|FindLocationClosesttoWorldLocation Spline (Transformation|GetActorLocation) "World") "World") "World"))))

(fn IncreaseCurrentSpeed
  (params (SpeedNormalized :type Float%20%28double-precision%29))
  (Variables|StatBase|Speed|SetCurrentSpeed (Math|Interpolation|FInterpTo (+ (* SpeedNormalized (Variables|StatBase|Speed|GetBaseMultiplierSpeed)) (Variables|StatBase|Speed|GetCurrentSpeed)) (Variables|StatBase|Speed|Forward|GetMaxSpeed) (Utilities|Time|GetWorldDeltaSeconds) (Variables|StatBase|Speed|Forward|GetThrottleSpeedInterp)))
  (return))

(fn DecreaseCurrentSpeed
  (params (SpeedNormalized :type Float%20%28double-precision%29))
  (Development|PrintText (Utilities|Text|FormatText "{s} Current Speed BackWard" SpeedNormalized) true true "(R=1.000000,G=0.432206,B=0.084933,A=1.000000)" 0.1)
  (Variables|StatBase|Speed|SetCurrentSpeed (Math|Interpolation|FInterpTo (+ (* SpeedNormalized (Variables|StatBase|Speed|GetBaseMultiplierSpeed)) (Variables|StatBase|Speed|GetCurrentSpeed)) (Variables|StatBase|Speed|Backward|GetMaxBackSpeed) (Utilities|Time|GetWorldDeltaSeconds) (Variables|StatBase|Speed|Backward|GetBackwardSpeedInterp)))
  (return))

(fn ApplyVelocity
  (bind _output_get (Variables|Physics|Velocity|SetFinalForces (+ (Variables|Physics|Velocity|GetShipForce) (Variables|Physics|Velocity|GetExternalForces))))
  (Physics|SetPhysicsLinearVelocity (Variables|Default|GetMainCollider) _output_get false "None"))

(fn ApplyDamping
  (bind _output_get (Variables|Physics|Velocity|SetFinalForces (- (Variables|Physics|Velocity|GetFinalForces) (* (Variables|Physics|Velocity|GetFinalForces) (Variables|Physics|OtherForces|GetDamping)))))
  (Physics|SetPhysicsLinearVelocity (Variables|Default|GetMainCollider) _output_get false "None")
  (bind _output_get_2 (Variables|StatBase|Speed|SetCurrentSpeed (- (Variables|StatBase|Speed|GetCurrentSpeed) (* (Variables|StatBase|Speed|GetCurrentSpeed) (Variables|Physics|OtherForces|GetDamping)))))
  (if (<= (Math|Float|Absolute(Float) _output_get_2) 1.0)
    (Variables|StatBase|Speed|SetCurrentSpeed 0.0)))

(fn ApplyForceShipForward
  (bind _currentspeed (Variables|StatBase|Speed|GetCurrentSpeed))
  (bind _maxbackspeed (Variables|StatBase|Speed|Backward|GetMaxBackSpeed))
  (bind _output_get (Variables|Physics|Velocity|SetShipForce (Math|Vector|ClampVectorSize (* (Transformation|GetActorForwardVector) (Math|Float|Clamp(Float) _currentspeed _maxbackspeed (Variables|StatBase|Speed|Forward|GetMaxSpeed))) _maxbackspeed _currentspeed)))
  (Development|PrintText (Utilities|Text|FormatText "Apply ShipForce {v}" (Utilities|String|ToString(Vector) _output_get)) true true "(R=0.000000,G=0.660000,B=1.000000,A=1.000000)" 0.0)
  (return))