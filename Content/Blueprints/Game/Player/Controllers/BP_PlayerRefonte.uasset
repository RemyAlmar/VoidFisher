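; Player ship that flies by physics, carries tools and collects data into an inventory.
; Each tick smooths input into speed, cone-limited direction and roll for BPCActorPhysicsMovement, driving camera FOV and sound.
; BPCToolShipManager handles the net and child-actor sucker, with the net changing camera arm length.
; Flow splines pull the ship toward their curve and, via velocity-tangent dot product, set a speed multiplier and directional VFX and rumble.
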(event Custom|OnUpgradeToolManager_Event
  (params (CurrentTool :type E_ToolShip%20Enum :default "NewEnumerator3"))
  ;[0 0.536 1 1 50] Event Feedback
)

(event Custom|FeedbackSpeed
  ;[0 0.536 1 1 50] Event Feedback
  (Camera|SetFieldOfView (Variables|Default|GetCameraController) (Math|Float|Lerp (Variables|Camera|GetFOVBase) (Variables|Camera|GetFOVSpeedMax) (Math|Float|SafeDivide (Variables|Movement|Speed|GetCurrentSpeed) (Variables|Movement|Speed|GetSpeedMax)))))

(event Custom|FeedbackOnHit
  (bind _forcefeedback (Variables|Default|GetForceFeedback))
  ;[0 0.536 1 1 50] Event Feedback
  (Audio|PlaySound2D "/Game/SFX/Sounds/Player/S_SFX_Collision.S_SFX_Collision" 1.0 1.0 0.0 "/Game/SFX/Sounds/Player/SC_Player.SC_Player" self false)
  (Class|ForceFeedbackComponent|SetForceFeedbackEffect _forcefeedback "/Game/Blueprints/AddOn/ForceFeedback/FFE_Hit.FFE_Hit")
  (Audio|Components|Audio|Play _forcefeedback 0.0)
  (Niagara|SpawnSystematLocation "/Game/VFX/Niagara/NS_ShipColision.NS_ShipColision" (Transformation|GetActorLocation)))

(event Custom|FeedBackOnFlow
  (bind _forcefeedback (Variables|Default|GetForceFeedback))
  ;[0 0.536 1 1 50] Event Feedback
  ;;[1 0 0.2077] Flow
  (Class|ForceFeedbackComponent|SetForceFeedbackEffect _forcefeedback "/Game/Blueprints/AddOn/ForceFeedback/FFE_IsInFlow.FFE_IsInFlow")
  (Audio|Components|Audio|Play _forcefeedback 0.0))

(event Custom|FeedbackOnFlowInBackDirection
  (bind _ns_oar (Variables|Default|GetNS_Oar))
  ;[0 0.536 1 1 50] Event Feedback
  ;;[1 0 0.2077] Flow
  (Class|NiagaraComponent|SetAsset _ns_oar "/Game/VFX/Niagara/NS_ShipInFlow.NS_ShipInFlow" true)
  (Niagara|SetNiagaraVariable(Float) _ns_oar "SpawnRate" 2e+02)
  (Class|ForceFeedbackComponent|SetIntensityMultiplier (Variables|Default|GetForceFeedback) 1.0))

(event Custom|FeedbackOnFlowInRightDirection
  (bind _ns_oar (Variables|Default|GetNS_Oar))
  ;[0 0.536 1 1 50] Event Feedback
  ;;[1 0 0.2077] Flow
  (Class|NiagaraComponent|SetAsset _ns_oar "/Game/VFX/Niagara/NS_AccelerationShip.NS_AccelerationShip" true)
  (Niagara|SetNiagaraVariable(Float) _ns_oar "SpawnRate" 2e+02)
  (Class|ForceFeedbackComponent|SetIntensityMultiplier (Variables|Default|GetForceFeedback) 0.5))

(event Custom|OnUseToolManager_Event
  (params (CurrentTool :type E_ToolShip%20Enum :default "NewEnumerator3"))
  ;[0 0.536 1 1 50] Event Feedback
)

(event Custom|OnUseSecondaryToolManager_Event
  (params (CurrentTool :type E_ToolShip%20Enum :default "NewEnumerator3"))
  ;[0 0.536 1 1 50] Event Feedback
)

(event Custom|OnActiveToolManager_Event
  (params (CurrentTool :type E_ToolShip%20Enum :default "NewEnumerator3"))
  ;[0 0.536 1 1 50] Event Feedback
  (switch Utilities|FlowControl|Switch|SwitchonE_ToolShip CurrentTool
    (:NewEnumerator2
      (Variables|Camera|Distance|SetTargetCameraPosition (Variables|Camera|Distance|GetCameraLengthNet)))))

(event Custom|OnDeactiveToolManager_Event
  (params (CurrentTool :type E_ToolShip%20Enum :default "NewEnumerator3"))
  ;[0 0.536 1 1 50] Event Feedback
  (switch Utilities|FlowControl|Switch|SwitchonE_ToolShip CurrentTool
    (:NewEnumerator2
      (Variables|Camera|Distance|SetTargetCameraPosition (Variables|Camera|Distance|GetCameraLengthBase)))))

(event Custom|OnUnlockToolManager_Event
  (params (CurrentTool :type E_ToolShip%20Enum :default "NewEnumerator3"))
  ;[0 0.536 1 1 50] Event Feedback
)

(event Collision|EventHit
  (params (MyComp :type Primitive%20Component%20Object%20Reference) (Other :type Actor%20Object%20Reference) (OtherComp :type Primitive%20Component%20Object%20Reference) (bSelfMoved :type Boolean) (HitLocation :type Vector :default "0, 0, 0") (HitNormal :type Vector :default "0, 0, 0") (NormalImpulse :type Vector :default "0, 0, 0") (Hit :type Hit%20Result%20Structure%20%28by%20ref%29))
  ;[1 0.7569 0] When Ship hit something
  (CallFunction|FeedbackonHit))

(event EventTick
  (params (DeltaSeconds :type Float%20%28single-precision%29))
  (bind _bpc_actorphysicsmovement (Variables|Default|GetBPC_ActorPhysicsMovement))
  (bind _bpc_actorphysicsmovement_2 (Variables|Default|GetBPC_ActorPhysicsMovement))
  ;[0 1 0.8061] Apply All (Direction, Rotation, Etc...)
  (Utilities|FlowControl|Sequence
    (:then_0
      (Variables|/Game/Blueprints/AddOn/Components/BPC_ActorPhysicsMovement.BPC_ActorPhysicsMovement_C|SetCurrentSpeed _bpc_actorphysicsmovement (Variables|Movement|Speed|GetCurrentSpeed))
      (Default|ApplyMovement _bpc_actorphysicsmovement)
      (Default|ApplyRotation _bpc_actorphysicsmovement_2)
      (Default|SetRollonSceneComp _bpc_actorphysicsmovement_2 (Variables|Default|GetSkeletalMesh) 4e+01 0.6)
      (Camera|ChangeTargetLength (Variables|Camera|Distance|GetTargetCameraPosition))
      (Audio|Components|Audio|SetVolumeMultiplier (Variables|Default|GetSFX_SpeedSound) (Variables|Movement|Speed|GetCurrentSpeed) :!class /Script/Engine.AudioComponent)
      (CallFunction|FeedbackSpeed))
    (:then_1
      (|SetCursorPosition)
      (|ApplyRollByInputs)
      (|ApplyDirection) ; Applique une direction via les inputs de Camera Look
      (|ModificationCurrentSpeed)
      (Development|PrintText (Utilities|Text|FormatText "{x} km/h" (Math|Float|Round (Math|Float|Absolute(Float) (/ (Variables|Movement|Speed|GetCurrentSpeed) 1e+01)))) true true "(R=1.000000,G=0.406524,B=0.006859,A=1.000000)" 0.0))))

(event EventFlowEnd
  ;[0 0.536 1 1 50] Event Feedback
  ;;[1 0 0.2077] Flow
  (Niagara|SetNiagaraVariable(Float) (Variables|Default|GetNS_Oar) "SpawnRate" 0.0)
  (Audio|Components|Audio|Stop (Variables|Default|GetForceFeedback)))

(event EventUpdateData
  (params (Data :type Map%20of%20E_CreatureType%20Enums%20to%20Structs :default "NewEnumerator4"))
  ;[0.1602 1 0.3842] Transition Data Inventory
  (Default|UpdateData (Variables|Default|GetHUD_Ship) Data)
  (Class|BPIInventory|UpdateData(Message) (Game|GetGameInstance) Data))

(event EventFlowStart
  (params (Spline :type Spline%20Component%20Object%20Reference) (BaseSpeed :type Float%20%28double-precision%29) (SlugSpeed :type Float%20%28double-precision%29) (SubsonicSpeed :type Float%20%28double-precision%29) (MagnetStrength :type Float%20%28double-precision%29) (Damping :type Float%20%28double-precision%29))
  ;[1 1 0.5583] Flow Influence
  (Utilities|FlowControl|Sequence
    (:then_0
      (Curve|SpeedinFlowDirection Spline BaseSpeed SlugSpeed SubsonicSpeed))
    (:then_1
      (bind _returnvalue (Curve|AttractPlayertoCurve Spline MagnetStrength Damping))))
  (Physics|SetPhysicsLinearVelocity (Variables|Default|GetRoot) _returnvalue true "None"))

(event EventAddData
  (params (Data :type S%20Creature%20Details%20Instanced%20Structure))
  ;[0.1602 1 0.3842] Transition Data Inventory
  (Default|AddData (Variables|Default|GetBPC_InventoryComponent) Data)
  (Audio|PlaySound2D "/Game/SFX/Sounds/Fish/S_Capture.S_Capture" 1.0 1.0 0.0 0 0))

(event EventMoveBack
  (params (Value :type Float%20%28double-precision%29))
  ;[0 1 0.8061] Apply All (Direction, Rotation, Etc...)
  (Variables|Private(Don'tModify)|SetTargetSpeed (* Value (Variables|Movement|Speed|GetSpeedMin)))
  (Variables|Private(Don'tModify)|SetIsAccelerate true))

(event EventMoveForward
  (params (Value :type Float%20%28double-precision%29))
  ;[0 1 0.8061] Apply All (Direction, Rotation, Etc...)
  (Variables|Private(Don'tModify)|SetTargetSpeed (* Value (Variables|Movement|Speed|GetSpeedMax)))
  (Variables|Private(Don'tModify)|SetIsAccelerate true))

(event EventBeginPlay
  ;[1 0.5064 0.8696] Play
  (Utilities|FlowControl|Sequence
    (:then_0
      ;;[1 0.4555 0] Initialize les outils (child Actor)
      (Default|Initialize (Variables|Components|GetBP_SuctionTriggerFish) (Variables|Default|GetRoot))
      (bind _asbp_game_instance (Utilities|Casting|CastToBP_GameInstance (Game|GetGameInstance)))
      (Variables|/Game/Blueprints/Data/BP_GameInstance.BP_GameInstance_C|SetPlayer _asbp_game_instance self))
    (:then_1
      ;;[0 1 0.5447] Ajoute les tools au toolship manager
      (Default|AddTool (Variables|Default|GetBPC_ToolShipManager) (Utilities|Enum|LiteralenumE_ToolShip "NewEnumerator2") (Variables|Default|GetBPC_NetTool))
      (Default|AddTool (Variables|Default|GetBPC_ToolShipManager) (Utilities|Enum|LiteralenumE_ToolShip "NewEnumerator0") (Actor|GetComponentbyClass (Variables|Components|GetBP_SuctionTriggerFish) "/Game/Blueprints/Game/Player/ToolsComponent/BPC_ToolBase.BPC_ToolBase_C"))
      (bind _asbp_hud_ship (Utilities|Casting|CastToBP_HUD_Ship (HUD|GetHUD (Game|GetPlayerController 0))))
      (Variables|Default|SetHUD_Ship _asbp_hud_ship)
      (Niagara|SetNiagaraVariable(Float) (Variables|Default|GetNS_Oar) "SpawnRate" 0.0)
      (|BindingToolShipManager))))

(event EventSetDirection
  (params (LookDirection :type Vector%202D%20Structure))
  ;[0.4203 0.3757 1] Set Direction & Roll
  (Variables|Private(Don'tModify)|SetCurrentInputDirection (+ LookDirection (Variables|Private(Don'tModify)|GetCurrentInputDirection))))

(event EventRoll
  (params (AxisValues :type Vector%202D%20Structure))
  ;[0.4203 0.3757 1] Set Direction & Roll
  (Variables|Private(Don'tModify)|SetRollTarget (+ (* (* (.x AxisValues) (Utilities|Time|GetWorldDeltaSeconds)) (Variables|Movement|Rotation|Roll|GetSpeedRoll)) (Variables|Private(Don'tModify)|GetRollTarget))))

(event EventBegintoStopSpeed
  ;[0 1 0.8061] Apply All (Direction, Rotation, Etc...)
  (Variables|Private(Don'tModify)|SetIsAccelerate false)
  (Variables|Private(Don'tModify)|SetTargetSpeed 0.0))

(event EventISelectTool
  (params (ToolSelected :type E_ToolShip%20Enum :default "NewEnumerator3"))
  ;[1 0.9883 0] Tools
  (Default|ToggleTool (Variables|Default|GetBPC_ToolShipManager) ToolSelected))

(event EventIUseTool
  ;[1 0.9883 0] Tools
  (Default|UseTool (Variables|Default|GetBPC_ToolShipManager)))

(event EventIUnlockTool
  (params (ToolToUnlock :type E_ToolShip%20Enum :default "NewEnumerator3"))
  ;[1 0.9883 0] Tools
  (Default|UnlockTool (Variables|Default|GetBPC_ToolShipManager) ToolToUnlock))

(event EventIUseSecondaryTool
  ;[1 0.9883 0] Tools
  (Default|UseSecondaryTool (Variables|Default|GetBPC_ToolShipManager)))

(fn ConstructionScript
  (Default|Initialization (Variables|Default|GetBPC_NetTool) (Variables|Default|GetNetCollider) (Variables|Default|GetAspiratorCenter) (Variables|Default|GetSM_Net))
  (bind _output_get (Variables|Camera|Distance|SetCameraLengthBase (Variables|/Script/Engine.SpringArmComponent|GetTargetArmLength (Variables|Default|GetSPA_Cam))))
  (Variables|Camera|Distance|SetTargetCameraPosition _output_get)
  (bind _output_get_2 (Variables|Camera|SetFOVBase (Variables|/Script/Engine.CameraComponent|GetFieldOfView (Variables|Default|GetCameraController))))
  (Variables|Camera|SetFOVSpeedMax (* _output_get_2 1.33))
  (bind _asbp_tool_thread_launcher (Utilities|Casting|CastToBP_ToolThreadLauncher (Variables|/Script/Engine.ChildActorComponent|GetChildActor (Variables|Default|GetSuctionTriggerfish))))
  (Variables|Components|SetBP_SuctionTriggerFish _asbp_tool_thread_launcher)
  (Variables|/Game/Blueprints/AddOn/Components/BPC_ActorPhysicsMovement.BPC_ActorPhysicsMovement_C|SetRotationRate (Variables|Default|GetBPC_ActorPhysicsMovement) (Variables|Movement|Rotation|GetRotationRate)))

(fn GetSplineDirection
  (params (Spline :type Spline%20Component%20Object%20Reference))
  (return (Math|Vector|Normalize (Spline|GetTangentatDistanceAlongSpline Spline (Class|SplineComponent|GetDistanceAlongSplineatLocation Spline (Spline|FindLocationClosesttoWorldLocation Spline (Transformation|GetActorLocation) "World") "World") "World"))))

(fn SpeedinFlowDirection
  (params (Spline :type Spline%20Component%20Object%20Reference) (Base%20Speed :type Float%20%28double-precision%29) (Slug%20Speed :type Float%20%28double-precision%29) (Huge%20Speed :type Float%20%28double-precision%29))
  (if (Variables|Movement|GetUseSensFlow)
    (bind _direction__normalize_ (Curve|GetSplineDirection Spline)) ; Renvoie la direction Normalized du point le plus proche dans la spline
    (Variables|Curve|SetIsInTheCourant%20!!! true)
    (bind _returnvalue (Physics|GetPhysicsLinearVelocity (Variables|Default|GetRoot) "None"))
    (if (and (> (Math|Vector|DotProduct _direction__normalize_ (Math|Vector|Normalize _returnvalue)) -0.1) (< (Math|Vector|DotProduct _direction__normalize_ (Math|Vector|Normalize _returnvalue)) 0.1)) ; Est perpendiculaire par rapport à la spline
      (Variables|StatBase|SetBaseMultiplierSpeed Base%20Speed)
      (return)
      (elif (> (Math|Vector|DotProduct _direction__normalize_ (Math|Vector|Normalize _returnvalue)) 0.0) ; va dans le bon sens de la spline
        (Variables|StatBase|SetBaseMultiplierSpeed Huge%20Speed :!label _label)
        (CallFunction|FeedbackonFlowinRightDirection)
        (return)
        (elif (< (Math|Vector|DotProduct _direction__normalize_ (Math|Vector|Normalize _returnvalue)) 0.0) ; va dans le sens inverse de la spline
          (Variables|StatBase|SetBaseMultiplierSpeed Slug%20Speed)
          (CallFunction|FeedbackonFlowinBackDirection)
          (return)
          (else
            (Development|PrintString "Il y a une couille dans le pâté, je répète, il y a une couille dans le pâté" true true "(R=20.000000,G=1.864536,B=0.000000,A=1.000000)" 15.0)))))
    (else
      (goto _label))))

(fn AttractPlayertoCurve
  (params (Spline :type Spline%20Component%20Object%20Reference) (Magnet :type Float%20%28double-precision%29) (Damping :type Float%20%28double-precision%29))
  (bind _returnvalue (Transformation|GetActorLocation))
  (bind _returnvalue_2 (Spline|FindLocationClosesttoWorldLocation Spline _returnvalue "World"))
  (return (* (* (Math|Vector|VectorLength (- _returnvalue _returnvalue_2)) (* (Math|Vector|Normalize (- _returnvalue_2 _returnvalue)) (* (Variables|Curve|GetFlowSpeedMultiplier) Magnet))) (Variables|StatBase|GetDamping))))

(fn ChangeTargetLength
  (params (TargetLength :type Float%20%28double-precision%29))
  (bind _spa_cam (Variables|Default|GetSPA_Cam))
  (Variables|/Script/Engine.SpringArmComponent|SetTargetArmLength _spa_cam (Math|Interpolation|FInterpTo (Variables|/Script/Engine.SpringArmComponent|GetTargetArmLength _spa_cam) TargetLength (Utilities|Time|GetWorldDeltaSeconds) (Variables|Camera|Distance|GetInterpSpeedCam)))
  (return))