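; Player ship controller that flies a physics-driven craft with a lagged camera, selectable net, bait and sucker tools, and creature data capture.
; Tick lerps velocity along a reference mesh's forward vector using a decaying speed value, tilts the ship with steering and scales turn rate by speed.
; Flow currents set speed by travel direction against the spline tangent and pull the ship toward the curve, with Niagara and force feedback.
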(event EventHorizontalRoll
  (params (AxisValue :type Float%20%28double-precision%29))
  ;[0.4203 0.3757 1] Roll Ship
  (Transformation|AddLocalRotation (Variables|Default|GetPointReferenceMesh) (Math|Rotator|MakeRotator (* AxisValue (Variables|Movement|Roll|GetRollPlayerSpeed)) 0.0 0.0) false false))

(event Collision|EventHit
  (params (MyComp :type Primitive%20Component%20Object%20Reference) (Other :type Actor%20Object%20Reference) (OtherComp :type Primitive%20Component%20Object%20Reference) (bSelfMoved :type Boolean) (HitLocation :type Vector :default "0, 0, 0") (HitNormal :type Vector :default "0, 0, 0") (NormalImpulse :type Vector :default "0, 0, 0") (Hit :type Hit%20Result%20Structure%20%28by%20ref%29))
  (bind _forcefeedback (Variables|Default|GetForceFeedback))
  ;[1 0.7569 0] When Ship hit something
  (Variables|Speed|SetSpeedDirection (Math|Interpolation|FInterpTo (Variables|Speed|GetSpeedDirection) 0.0 0.5 5e+01)) ; On ralentit la vitesse du vaisseau j'uqu'à 0 (est compensé par la réaccelération du vaisseau)
  ;;[0.5654 1 0.6811] Feedback
  (Audio|PlaySound2D "/Game/SFX/Sounds/Player/S_SFX_Collision.S_SFX_Collision" 1.0 1.0 0.0 "/Game/SFX/Sounds/Player/SC_Player.SC_Player" self false)
  (Class|ForceFeedbackComponent|SetForceFeedbackEffect _forcefeedback "/Game/Blueprints/AddOn/ForceFeedback/FFE_Hit.FFE_Hit")
  (Audio|Components|Audio|Play _forcefeedback 0.0))

(event EventTick
  (params (DeltaSeconds :type Float%20%28single-precision%29))
  ;[0.9969 1 0.5568] Move Forward
  (Utilities|FlowControl|Sequence
    (:then_0
      (CallFunction|MoveShipbySpeed) ; Deplacement du vaisseau
      (Audio|Components|Audio|SetVolumeMultiplier (Variables|Default|GetSFX_SpeedSound) (Variables|Speed|GetSpeedDirection) :!class /Script/Engine.AudioComponent))
    (:then_1
      (CallFunction|RollShip DeltaSeconds (.x (stale EventCameraLook LookDirection)) (.y (stale EventCameraLook LookDirection))) ; Gère le roll automatique du vaisseau quand kle vaisseau doit tourner dans une direction
      (Transformation|SetActorTransform (Transformation|GetWorldTransform (Variables|Default|GetPointReferenceMesh))) ; pansement pour le root qui a perdu ses parents
    )
    (:then_2
      (Variables|Speed|SetSpeedDirection (Math|Interpolation|FInterpTo (Variables|Speed|GetSpeedDirection) 0.0 DeltaSeconds 0.5)) ; le vaisseau ralentit petit à petit si aucun input n'est activé (input qui influe la vitesse)
      (CallFunction|ChangeCameraSpeedbySpeedShip) ; la caméra est plus rapide lorsque le vaisseau est à l'arrêt et au contraire plus lente quand le vaisseau est rapide
    )
    (:then_3
      (if (<= (Variables|Speed|GetSpeedDirection) 0.1) ; si le vaisseau est a moins de 10% de sa vitesse
        (Variables|Speed|SetShipStop (Math|Interpolation|FInterpTo (Variables|Speed|GetShipStop) 0.0 DeltaSeconds 5.0)) ; le vaisseau s'arrête
        (else
          (Variables|Speed|SetShipStop (Math|Interpolation|FInterpTo (Variables|Speed|GetShipStop) 1.0 DeltaSeconds 1.0)) ; sinon il avance (ship stop : 1 avance / 0 s'arrête
        )))
    (:then_4
      (if (Variables|Default|GetIsInTheCourant%20!!!)
        (Variables|Speed|SetSpeedDirection (* 1.0 (Variables|Default|GetFlowSpeedMultiplayer)))
        (Variables|Default|SetIsInTheCourant%20!!! false)))))

(event EventFlowEnd
  ;[1 1 0.5583] Flow Influence
  ;;[0.5654 1 0.6811] Feedback
  (|StopFeedBack))

(event EventUpdateData
  (params (Data :type Map%20of%20E_CreatureType%20Enums%20to%20Structs :default "NewEnumerator3"))
  ;[0.1602 1 0.3842] Transition Data Inventory
  (Default|UpdateData (Variables|Default|GetHUD_Ship) Data))

(event EventFlowStart
  (params (Spline :type Spline%20Component%20Object%20Reference) (BaseSpeed :type Float%20%28double-precision%29) (SlugSpeed :type Float%20%28double-precision%29) (SubsonicSpeed :type Float%20%28double-precision%29) (MagnetStrength :type Float%20%28double-precision%29) (Damping :type Float%20%28double-precision%29))
  (bind _forcefeedback (Variables|Default|GetForceFeedback))
  ;[1 1 0.5583] Flow Influence
  (Utilities|FlowControl|Sequence
    (:then_0
      (bind _pointreferencemesh (CallFunction|SpeedinFlowDirection Spline BaseSpeed SlugSpeed SubsonicSpeed)))
    (:then_1
      (bind _returnvalue (CallFunction|AttractPlayertoCurve Spline MagnetStrength Damping))))
  (Physics|SetPhysicsLinearVelocity _pointreferencemesh _returnvalue true "None")
  ;;[0.5654 1 0.6811] Feedback
  (Class|ForceFeedbackComponent|SetForceFeedbackEffect _forcefeedback "/Game/Blueprints/AddOn/ForceFeedback/FFE_IsInFlow.FFE_IsInFlow")
  (Audio|Components|Audio|Play _forcefeedback 0.0))

(event EventAddData
  (params (CreatureType :type E_CreatureType%20Enum :default "NewEnumerator3") (Data :type S%20Catcheable%20Data%20Structure))
  ;[0.1602 1 0.3842] Transition Data Inventory
  (Default|AddData (Variables|Default|GetBP_InventoryComponent) CreatureType Data)
  (Audio|PlaySound2D "/Game/SFX/Sounds/Fish/S_Capture.S_Capture" 1.0 1.0 0.0 0 0))

(event EventBeginPlay
  ;[1 0.5064 0.8696] Play
  (Default|AddTool (Variables|Default|GetBP_ToolShipManager) (Utilities|Enum|LiteralenumE_ToolShip "NewEnumerator2") (Variables|Default|GetBP_NetTool))
  (Default|AddTool (Variables|Default|GetBP_ToolShipManager) (Utilities|Enum|LiteralenumE_ToolShip "NewEnumerator1") (Variables|Default|GetBP_BaitTool))
  (Default|AddTool (Variables|Default|GetBP_ToolShipManager) (Utilities|Enum|LiteralenumE_ToolShip "NewEnumerator0") (Variables|Default|GetBP_SuckerTool))
  (bind _asbp_hud_ship (Utilities|Casting|CastToBP_HUD_Ship (HUD|GetHUD (Game|GetPlayerController 0))))
  (Variables|Default|SetHUD_Ship _asbp_hud_ship)
  (Niagara|SetNiagaraVariable(Float) (Variables|Default|GetNS_ShipInFlow) "SpawnRate" 0.0))

(event EventISelectTool
  (params (ToolSelected :type E_ToolShip%20Enum :default "NewEnumerator3"))
  ;[1 0.9883 0] Tools
  (Default|ToggleTool (Variables|Default|GetBP_ToolShipManager) ToolSelected))

(event EventIUseTool
  ;[1 0.9883 0] Tools
  (Default|UseTool (Variables|Default|GetBP_ToolShipManager)))

(event EventCameraLook
  (params (LookDirection :type Vector%202D%20Structure))
  (bind _current_rotation_speed (Variables|Movement|GetCurrent%20Rotation%20Speed))
  ;[0.4203 0.3757 1] Set Rotation
  (Transformation|AddLocalRotation (Variables|Default|GetPointReferenceMesh) (Math|Rotator|MakeRotator 0.0 (* (* (.y LookDirection) _current_rotation_speed) -1.0) (* (.x LookDirection) _current_rotation_speed)) false false) ; Fait tourner le routeur qui fera tourner avec du lag la caméra et le vaisseau
)

(event EventIUnlockTool
  (params (ToolToUnlock :type E_ToolShip%20Enum :default "NewEnumerator3"))
  ;[1 0.9883 0] Tools
  (Default|UnlockTool (Variables|Default|GetBP_ToolShipManager) ToolToUnlock))

(event EventMoveBack
  (params (Value :type Float%20%28double-precision%29))
  ;[0.9969 1 0.5568] Move Forward
  (Variables|Speed|SetSpeedDirection (Math|Interpolation|FInterpTo (Variables|Speed|GetSpeedDirection) 0.0 (Utilities|Time|GetWorldDeltaSeconds) 1.0)) ; Marche pas pour le moment car creer un bug de caméra à cause des double spring arm
)

(event EventMoveForward
  (params (Value :type Float%20%28double-precision%29))
  ;[0.9969 1 0.5568] Move Forward
  (Variables|Speed|SetSpeedDirection (Math|Interpolation|FInterpTo (Variables|Speed|GetSpeedDirection) Value (Utilities|Time|GetWorldDeltaSeconds) 1.0)) ; On lerp la vitesse jusqu'à 1 (multiplication par rapport à la vitesse max)
)

(event EventIUseSecondaryTool
  ;[1 0.9883 0] Tools
  (Default|UseSecondaryTool (Variables|Default|GetBP_ToolShipManager))
  (Audio|PlaySound2D "/Game/SFX/Sounds/Player/S_SortieOutil.S_SortieOutil" 1.0 1.0 0.0 0 0))

(fn ConstructionScript
  (bind _bp_nettool (Variables|Default|GetBP_NetTool))
  (Variables|/Game/Blueprints/Game/Player/Tools/BP_NetTool.BP_NetTool_C|SetNetCollider _bp_nettool (Variables|Default|GetNetCollider))
  (Default|Initialize _bp_nettool)
  (Variables|/Game/Blueprints/Game/Player/Tools/BP_ToolLauncher.BP_ToolLauncher_C|SetSpawnTransform (Variables|Default|GetBP_BaitTool) (Variables|Default|GetBH_Launcher))
  (Variables|/Game/Blueprints/Game/Player/Tools/BP_ToolLauncher.BP_ToolLauncher_C|SetSpawnTransform (Variables|Default|GetBP_SuckerTool) (Variables|Default|GetBH_Launcher)))

(fn RollShip
  (params (DeltaTime :type Float%20%28single-precision%29) (Right%20Float :type Float%20%28double-precision%29) (Up%20Float :type Float%20%28double-precision%29))
  (if (!= Right%20Float 0.0) ; Si le roll up (haut et bas) est différent de 0 alors
    (if (> (Variables|Speed|GetShipStop) 0.01) ; Si le vaisseau n'a pas une vitesse null (on a forcé l'arrêt du vaisseau avec le ship stop)
      (if (> (Variables|Speed|GetSpeedDirection) 0.0) ; si le vaisseau est en mouvement
        (|PositiveRoll DeltaTime Right%20Float Up%20Float) ; On fait un roll par rapport à la rotation de la camera
        (return)
        (else
          (|NegativeRoll Right%20Float DeltaTime Up%20Float) ; on fait un roll dans l'autre sens
          (return)))
      (else
        (|ResetRotationto0 (Variables|Default|GetSPA_Ship) DeltaTime) ; Remet le Roll du vaisseau à 0 avec un lerp de manière smooth
        (return)))
    (else
      (|ResetRoll (Variables|Default|GetSPA_Ship) DeltaTime) ; Remet le Roll du vaisseau à 0 avec un lerp de manière smooth
      (return))))

(fn MoveShipbySpeed
  (bind _pointreferencemesh (Variables|Default|GetPointReferenceMesh))
  (bind _returnvalue (Physics|GetPhysicsLinearVelocity _pointreferencemesh "None"))
  (Physics|SetPhysicsLinearVelocity _pointreferencemesh (Math|Vector|Lerp(Vector) _returnvalue (* (Math|Vector|GetForwardVector (Variables|Default|GetPointReferenceMesh)) (* (* (Variables|Speed|GetSpeedDirection) (* (Variables|StatBase|GetBaseMultiplierSpeed) (Variables|Speed|GetSpeedTarget))) (Variables|Speed|GetShipStop))) 0.01) false "None"))

(fn Brake
  (CallFunction|DecreaseValueinTime (Variables|Speed|GetSpeedDirection) 0.0 0.0 1.0 0.0 0.0 false)
  (CallFunction|DecreaseValueExp 0.0 1.0 1.0 1.1 0.0))

(fn ChangeCameraSpeedbySpeedShip
  (Variables|Movement|SetCurrent%20Rotation%20Speed (Math|Float|Clamp(Float) (Math|Float|SafeDivide 0.4 (Math|Float|Absolute(Float) (Variables|Speed|GetSpeedDirection))) 1.0 1.5)))

(fn GetSplineDirection
  (params (Spline :type Spline%20Component%20Object%20Reference))
  (return (Math|Vector|Normalize (Spline|GetTangentatDistanceAlongSpline Spline (Class|SplineComponent|GetDistanceAlongSplineatLocation Spline (Spline|FindLocationClosesttoWorldLocation Spline (Transformation|GetWorldLocation (Variables|Default|GetPointReferenceMesh)) "World") "World") "World"))))

(fn SpeedinFlowDirection
  (params (Spline :type Spline%20Component%20Object%20Reference) (Base%20Speed :type Float%20%28double-precision%29) (Slug%20Speed :type Float%20%28double-precision%29) (Huge%20Speed :type Float%20%28double-precision%29))
  (bind _pointreferencemesh (Variables|Default|GetPointReferenceMesh))
  (bind _direction__normalize_ (CallFunction|GetSplineDirection Spline)) ; Renvoie la direction Normalized du point le plus proche dans la spline
  (Variables|Default|SetIsInTheCourant%20!!! true)
  (bind _returnvalue (Physics|GetPhysicsLinearVelocity _pointreferencemesh "None"))
  (if (and (> (Math|Vector|DotProduct (Math|Vector|Normalize _returnvalue) _direction__normalize_) -0.1) (< (Math|Vector|DotProduct (Math|Vector|Normalize _returnvalue) _direction__normalize_) 0.1)) ; Est perpendiculaire par rapport à la spline
    (Variables|Default|SetFlowSpeedMultiplayer Base%20Speed)
    (elif (> (Math|Vector|DotProduct (Math|Vector|Normalize _returnvalue) _direction__normalize_) 0.0) ; va dans le bon sens de la spline
      (Variables|Default|SetFlowSpeedMultiplayer Huge%20Speed)
      ;[0.5654 1 0.6811] Feedback
      (|SetFeedBacks)
      (elif (< (Math|Vector|DotProduct (Math|Vector|Normalize _returnvalue) _direction__normalize_) 0.0) ; va dans le sens inverse de la spline
        (Variables|Default|SetFlowSpeedMultiplayer Slug%20Speed)
        (|SetFeedBack)
        (else
          (Development|PrintString "Il y a une couille dans le pâté, je répète, il y a une couille dans le pâté" true true "(R=20.000000,G=1.864536,B=0.000000,A=1.000000)" 15.0)))))
  (return _pointreferencemesh))

(fn AttractPlayertoCurve
  (params (Spline :type Spline%20Component%20Object%20Reference) (Magnet :type Float%20%28double-precision%29) (Damping :type Float%20%28double-precision%29))
  (bind _pointreferencemesh (Variables|Default|GetPointReferenceMesh))
  (bind _returnvalue (Transformation|GetWorldLocation _pointreferencemesh))
  (bind _returnvalue_2 (Spline|FindLocationClosesttoWorldLocation Spline _returnvalue "World"))
  (return (* Damping (* (* (Math|Vector|Normalize (- _returnvalue_2 (Transformation|GetWorldLocation (Variables|Default|GetPointReferenceMesh)))) (* (Variables|Default|GetFlowSpeedMultiplayer) Magnet)) (Math|Vector|VectorLength (- _returnvalue _returnvalue_2))))))