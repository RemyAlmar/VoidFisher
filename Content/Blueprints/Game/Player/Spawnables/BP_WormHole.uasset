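; BP_WormHole is a timed wormhole actor that teleports actors with BPC_ActorPhysicsMovement to a linked twin.
; It spawns its exit at a random point near the edge of a radius, trace-clamped to blocking hits, and cross-links both.
; Overlap moves the actor, using CanTeleport to prevent bounce-back, and starts closing.
; A Niagara effect shows the portal, a Timeline drives its closing Power, and destruction closes the partner.
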(event OnComponentBeginOverlap(Overlap)
  (params (OverlappedComponent :type Primitive%20Component%20Object%20Reference) (OtherActor :type Actor%20Object%20Reference) (OtherComp :type Primitive%20Component%20Object%20Reference) (OtherBodyIndex :type Integer) (bFromSweep :type Boolean) (SweepResult :type Hit%20Result%20Structure%20%28by%20ref%29))
  (Variables|Default|GetWormHole_Exit
    (:then
      (Utilities|IsValid (Actor|GetComponentbyClass OtherActor "/Game/Blueprints/AddOn/Components/BPC_ActorPhysicsMovement.BPC_ActorPhysicsMovement_C")
        (:Is%20Valid
          (CallFunction|TeleportonExitWormHole OtherActor)
          (CallFunction|OnCloseWormHole))))
    (:else)))

(event Custom|CreateExitWormHole
  (params (Distance :type Float%20%28double-precision%29))
  (Utilities|FlowControl|Delay 0.1)
  (CallFunction|CreationExitWormHole Distance))

(event Custom|OnCloseWormHole
  (bind _power (Timeline|Timeline Play)
    (:Update
      (Niagara|SetNiagaraVariable(Float) (stale EventBeginPlay _returnvalue_2) "Power" _power))
    (:Finished
      (Actor|DestroyActor))))

(event EventBeginPlay
  (bind _returnvalue (Transformation|GetActorTransform))
  (bind _duration (Variables|Default|GetDuration))
  (bind _returnvalue_2 (Niagara|SpawnSystematLocation "/Game/VFX/Niagara/Fish/NS_Wormhole.NS_Wormhole" (.location _returnvalue) (.rotation _returnvalue) "1.000000,1.000000,1.000000" true true "AutoRelease"))
  (Niagara|SetNiagaraVariable(Float) _returnvalue_2 "Power" 1.0)
  (Niagara|SetNiagaraVariable(Float) _returnvalue_2 "Loop Duration" _duration)
  (Niagara|SetNiagaraVariable(Float) _returnvalue_2 "SpriteSizeMultiplayer" (Math|Vector|GetMaxElement (.scale _returnvalue)))
  (Utilities|FlowControl|Delay _duration)
  (Actor|DestroyActor))

(event EventDestroyed
  (bind _wormhole_exit (Variables|Default|GetWormHole_Exit)
    (:then
      (CallFunction|OnCloseWormHole _wormhole_exit))
    (:else)))

(fn ConstructionScript)

(fn CreationExitWormHole
  (params (Radius :type Float%20%28double-precision%29))
  (bind _returnvalue (Transformation|GetActorLocation))
  (bind _wormhole_exit (Variables|Default|GetWormHole_Exit)
    (:then
      (Actor|DestroyActor _wormhole_exit)
      (Variables|Default|SetWormHole_Exit 0))
    (:else
      _))
  (LocalVariables|SetCurrentLocation (CallFunction|GetRandomPointinSphere _returnvalue 0.85 Radius 1.0))
  (LocalVariables|SetCurrentRotation (Math|Conversions|RotationFromXVector (Math|Vector|GetUnitDirection(Vector) _returnvalue (LocalVariables|GetCurrentLocation))))
  (bind _outhit (Collision|LineTraceByChannel (Transformation|GetActorLocation) (LocalVariables|GetCurrentLocation) "TraceTypeQuery3" false 0 "None"))
  (if (.bBlockingHit (Collision|BreakHitResult _outhit))
    (LocalVariables|SetCurrentLocation (.ImpactPoint (Collision|BreakHitResult _outhit))))
  (bind _returnvalue_2 (Game|SpawnActorfromClass "BP_WormHole_C" (Math|Transform|MakeTransform (LocalVariables|GetCurrentLocation) (LocalVariables|GetCurrentRotation) (Transformation|GetActorScale3D)) "Undefined" "MultiplyWithRoot" 0 0))
  (bind _output_get (Variables|Default|SetWormHole_Exit _returnvalue_2))
  (Variables|BP_WormHole_C|SetWormHole_Exit _output_get self)
  (return))

(fn TeleportonExitWormHole
  (params (ActorTarget :type Actor%20Object%20Reference))
  (bind _wormhole_exit (Variables|Default|GetWormHole_Exit))
  (if (Variables|Default|GetCanTeleport)
    (Variables|BP_WormHole_C|SetCanTeleport _wormhole_exit false)
    (Transformation|SetActorLocationAndRotation ActorTarget (Transformation|GetActorLocation _wormhole_exit) (Transformation|GetActorRotation _wormhole_exit) true)
    (else
      (Variables|Default|SetCanTeleport true))))