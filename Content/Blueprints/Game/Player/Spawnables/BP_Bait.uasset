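; BP_Bait is a player-spawned bait projectile that lures a predator creature of a matching size and puts it to sleep.
; Its detection sphere, scaled by size effects, registers the bait as prey with one matching BPC_Predator at a time through event dispatcher calls.
; When that creature hits it, the bait fires its projectile effect and destroys itself.
; Removal from the hunt or destruction clears the predator link.
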(event OnComponentBeginOverlap(SenseDetection)
  (params (OverlappedComponent :type Primitive%20Component%20Object%20Reference) (OtherActor :type Actor%20Object%20Reference) (OtherComp :type Primitive%20Component%20Object%20Reference) (OtherBodyIndex :type Integer) (bFromSweep :type Boolean) (SweepResult :type Hit%20Result%20Structure%20%28by%20ref%29))
  (bind _returnvalue (Actor|GetComponentbyClass OtherActor "/Game/Blueprints/AddOn/Components/BPC_Predator.BPC_Predator_C"))
  ;[0.7294 0.5787 1] Je t'appate mon ptit Remy (g du jus de banane viens dans mon camion blanc) :3
  (Variables|Default|GetActorBaited
    (:then)
    (:else
      (Utilities|IsValid _returnvalue
        (:Is%20Valid
          (if (CallFunction|IsCreatureSizetoBait (Variables|/Game/Blueprints/AddOn/Components/BPC_Predator.BPC_Predator_C|GetSizeSelf _returnvalue)) ; Si la créature qui la suit a une taille égale à elle
            (EventDispatchers|BindEventtoEDRemovePreytoHunt _returnvalue (EventDispatchers|CreateEvent :!event Custom|RemoveSelfFromHunt))
            (Default|CallEDAddPreytoHunt _returnvalue self)
            (Variables|Default|SetActorBaited OtherActor)))))))

(event OnComponentHit(RootCollider)
  (params (HitComponent :type Primitive%20Component%20Object%20Reference) (OtherActor :type Actor%20Object%20Reference) (OtherComp :type Primitive%20Component%20Object%20Reference) (NormalImpulse :type Vector :default "0, 0, 0") (Hit :type Hit%20Result%20Structure%20%28by%20ref%29))
  ;[0.2555 1 0.7775] Il s'est fait bouffer
  (if (== (Variables|Default|GetActorBaited) OtherActor)
    (Default|CallEDActiveProjectileEffect)
    (Actor|DestroyActor)))

(event Custom|RemoveSelfFromHunt
  (params (PreyToRemoveFromHunt :type Actor%20Object%20Reference))
  (if (== PreyToRemoveFromHunt self)
    (bind _actorbaited (Variables|Default|GetActorBaited)
      (:then
        (EventDispatchers|UnbindallEventsfromEDRemovePreytoHunt (Actor|GetComponentbyClass _actorbaited "/Game/Blueprints/AddOn/Components/BPC_Predator.BPC_Predator_C"))
        (Variables|Default|SetActorBaited 0))
      (:else))))

(event EventDestroyed
  ;[0.3769 1 0] Destruction subatomique
  (bind _actorbaited (Variables|Default|GetActorBaited)
    (:then
      (Default|CallEDRemovePreytoHunt (Actor|GetComponentbyClass _actorbaited "/Game/Blueprints/AddOn/Components/BPC_Predator.BPC_Predator_C") self)
      (|CallParentFunction))
    (:else)))

(event EventEDActiveProjectileEvent
  (bind _actorbaited (Variables|Default|GetActorBaited)
    (:then
      (bind _asbp_creature_generic (Utilities|Casting|CastToBP_CreatureGeneric _actorbaited))
      (Default|CallEDHavetoSleep _asbp_creature_generic)
      (|CallParentFunction))
    (:else)))

(event EventEDSecondaryActionProjectileEvent
  (|CallParentFunction))

(fn ConstructionScript
  (Components|Sphere|SetSphereRadius (Variables|Default|GetSenseDetection) (Variables|Default|GetSenseDetectionRadius) true)
  (|CallParentFunction))

(fn ChangeFloatStatbyMultiplier
  (params (RefValue :type Float%20%28double-precision%29%20%28by%20ref%29) (Multiplier :type Float%20%28double-precision%29))
  (|CallParentFunction RefValue Multiplier)
  (return))

(fn IsCreatureSizetoBait
  (params (CreatureSize :type Byte))
  (return (== CreatureSize (Variables|Default|GetCreatureToBait))))

(fn ChangeSizeEffect
  (params (SizeMultiplier :type Float%20%28double-precision%29))
  (bind _sensedetectionradius (Variables|Default|GetSenseDetectionRadius))
  (|SetBy-RefVar _sensedetectionradius (* _sensedetectionradius SizeMultiplier))
  (Components|Sphere|SetSphereRadius (Variables|Default|GetSenseDetection) _sensedetectionradius true)
  (|CallParentFunction SizeMultiplier))