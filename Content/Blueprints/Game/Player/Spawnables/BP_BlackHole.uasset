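; BP_BlackHole is a player-spawnable projectile that turns into a stationary black hole with its own gravity field.
; On the bound secondary-action projectile event it stops physics, hides the capsule, reveals the black hole and enables the BPGravity component's tick.
; Construction passes two spheres to BPGravity as influence and stop-influence areas.
; Helper functions scale both radii and set or read the atmosphere gravity force.
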(event EventBeginPlay
  (EventDispatchers|BindEventtoEDSecondaryActionProjectile (EventDispatchers|CreateEvent :!event EDSecondaryActionProjectileEvent)))

(event EventEDSecondaryActionProjectileEvent
  (bind _rootcollider (Variables|Default|GetRootCollider))
  (Physics|SetPhysicsLinearVelocity _rootcollider "0, 0, 0" false "None")
  (Physics|SetSimulatePhysics _rootcollider false)
  (Rendering|SetVisibility (Variables|Default|GetCapsule) false false)
  (Rendering|SetVisibility (Variables|Default|GetBlackHole) true true)
  (Components|Tick|SetComponentTickEnabled (Variables|Default|GetBP_Gravity) true))

(fn ConstructionScript
  (Default|SetInfluenceSphere (Variables|Default|GetBP_Gravity) (Variables|Default|GetInfluenceOverlap) (Variables|Default|GetStopInfluence)))

(fn ChangeGlobalRadius
  (params (Multiplier :type Float%20%28single-precision%29))
  (Default|ChangeAtmosphereRadius (Variables|Default|GetBP_Gravity) (* (Variables|/Script/Engine.SphereComponent|GetSphereRadius (Variables|Default|GetInfluenceOverlap)) Multiplier))
  (Default|ChangeGroundRadius (Variables|Default|GetBP_Gravity) (* (Variables|/Script/Engine.SphereComponent|GetSphereRadius (Variables|Default|GetStopInfluence)) Multiplier)))

(fn ChangeGravityPower
  (params (AtmosphereGravityForce :type Float%20%28double-precision%29))
  (Variables|/Game/Blueprints/AddOn/Components/BPC_Gravity.BPC_Gravity_C|SetAtmosphereGravityForce (Variables|Default|GetBP_Gravity) AtmosphereGravityForce))

(fn GetCurrentGravityPower
  (return (Variables|/Game/Blueprints/AddOn/Components/BPC_Gravity.BPC_Gravity_C|GetAtmosphereGravityForce (Variables|Default|GetBP_Gravity))))