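; BP_Sucker is a launched suction tool on a cable that grapples onto anchors, extending a parent spawnable.
; Launch and target events toggle its grappling hook component, whose hook, unhook and physics events update target state and physics.
; Mid-launch hits without an active anchor play failure sound and particles.
; A missed target or unhook triggers cable bring-back through the tool thread parent; debug prints remain.
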(event EDonPhysicsChanged(BPC_GrapplingHook)
  (params (CurrentPhysics :type Boolean))
  (CallFunction|SetSimulatePhysics CurrentPhysics)
  (Development|PrintText (Utilities|Text|FormatText "Ah bah ca change ici en fait {x}" CurrentPhysics) true true "(R=0.092553,G=1.000000,B=0.270153,A=1.000000)" 1e+01))

(event OnComponentHit(RootCollider)
  (params (HitComponent :type Primitive%20Component%20Object%20Reference) (OtherActor :type Actor%20Object%20Reference) (OtherComp :type Primitive%20Component%20Object%20Reference) (NormalImpulse :type Vector :default "0, 0, 0") (Hit :type Hit%20Result%20Structure%20%28by%20ref%29))
  (bind _returnvalue (Actor|GetComponentbyClass OtherActor "/Game/Blueprints/AddOn/Components/BPC_AnchorManager.BPC_AnchorManager_C"))
  (if (Variables|Default|GetLaunched)
    (Utilities|IsValid _returnvalue
      (:Is%20Valid
        (if (not (Default|GetAnchorsIsActive _returnvalue))
          (CallFunction|SetTargetReached false :!label _label)
          (Audio|SpawnSoundatLocation "/Game/SFX/Sounds/NEW_OGG/Ventouse/SFX_SuckerNoTouch.SFX_SuckerNoTouch" (Transformation|GetWorldLocation (Variables|Default|GetRootCollider)) "0, 0, 0" 0.5 1.0 0.0 0 0)
          (Niagara|SpawnSystemAttached "/Game/VFX/Niagara/Player/NS_PlungeColision.NS_PlungeColision" (Variables|Default|GetRootCollider) "None" "0, 0, 0" "0, 0, 0" "KeepRelativeOffset" true)))
      (:Is%20Not%20Valid
        (goto _label)))))

(event EDonPhysicsActivated(BPC_GrapplingHook)
  (Default|CallEDonPhysicsActivated))

(event EDonPhysicsDeactivated(BPC_GrapplingHook)
  (Default|CallEDonPhysicsDeactivated))

(event EDHookonAnchor(BPC_GrapplingHook)
  (CallFunction|SetTargetReached true)
  (Audio|PlaySound2D "/Game/SFX/Sounds/NEW_OGG/Ventouse/SFX_SuckerTouch_Cue.SFX_SuckerTouch_Cue" 1.0 1.0 0.0 0 0))

(event EDCurrentlyHooked(BPC_GrapplingHook))

(event EDRemoveHookonAnchor(BPC_GrapplingHook)
  (bind _bpc_toolthreadparent (Variables|Default|GetBPC_ToolThreadParent))
  (if (Variables|/Game/Blueprints/Game/Player/ToolsComponent/BPC_ToolThread.BPC_ToolThread_C|GetBringBackCable _bpc_toolthreadparent)
    _
    (else
      (Default|EDStarttoBringBackEvent _bpc_toolthreadparent)))
  (CallFunction|SetTargetReached false))

(event EventTick
  (params (DeltaSeconds :type Float%20%28single-precision%29))
  (|CallParentFunction DeltaSeconds)
  (Development|PrintText (Utilities|Text|FormatText "{x} is physiqued" (Physics|IsSimulatingPhysics (Variables|Default|GetRootCollider) "None")) true true "(R=0.000000,G=1.000000,B=0.127254,A=1.000000)" 0.0))

(event EventEDonLaunchedEvent
  (|CallParentFunction)
  (Variables|/Game/Blueprints/AddOn/Components/BPC_GrapplingHook.BPC_GrapplingHook_C|SetCanHook (Variables|Default|GetBPC_GrapplingHook) (Variables|Default|GetLaunched)))

(event EventEDonTargetMissingEvent
  (|CallParentFunction)
  (Default|EDStarttoBringBackEvent (Variables|Default|GetBPC_ToolThreadParent)))

(event EventEDonTargetReachedEvent
  (|CallParentFunction)
  (Variables|/Game/Blueprints/AddOn/Components/BPC_GrapplingHook.BPC_GrapplingHook_C|SetCanHook (Variables|Default|GetBPC_GrapplingHook) false))

(event EventEDIsReplaceEvent
  (|CallParentFunction)
  (Niagara|SpawnSystemAttached "/Game/VFX/Niagara/Player/NS_Shoot.NS_Shoot" (Variables|Default|GetRootCollider) "None" "0.000000,0.000000,-25.000000" "0, 0, 0" "KeepRelativeOffset" true)
  (CallFunction|SetTargetReached false))

(event EventEDonStartBringBackEvent
  (Default|EDRemoveHookonAnchorEvent (Variables|Default|GetBPC_GrapplingHook))
  (Variables|/Game/Blueprints/AddOn/Components/BPC_GrapplingHook.BPC_GrapplingHook_C|SetCanHook (Variables|Default|GetBPC_GrapplingHook) false)
  (Development|PrintText "Balala wtf"))

(fn ConstructionScript)

(fn Initialize
  (params (SizeMultiplier :type Float%20%28single-precision%29) (PowerMultiplier :type Float%20%28double-precision%29) (NewLifeTime :type Float%20%28double-precision%29) (NewTriggerTime :type Float%20%28double-precision%29) (ToolThreadParent :type BPC%20Tool%20Thread%20Object%20Reference))
  (|CallParentFunction SizeMultiplier PowerMultiplier NewLifeTime NewTriggerTime ToolThreadParent)
  (bind _output_get (Variables|Default|SetBPC_ToolThreadParent ToolThreadParent))
  (EventDispatchers|BindEventtoEDStarttoBringBack _output_get (EventDispatchers|CreateEvent :!event EDonStartBringBackEvent)))