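; Base player projectile actor, initialized with power, size, lifetime and trigger-time values plus a parent tool thread; the size effect is an empty stub.
; Tick runs an optional one-shot timer for two-stage activation and optional lifetime destruction, and rotates the detached, physics-simulated projectile along its velocity through BPCActorPhysicsMovement.
; Setters for launched, target and physics state detect changes and raise events that relay to event dispatchers.
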(event Custom|ED_ActiveProjectile_Event
  (Default|CallEDActiveProjectileEffect))

(event Custom|ED_OnLaunched_Event
  (Default|CallEDonLaunched))

(event Custom|ED_OnPhysicsActivated_Event
  (Default|CallEDonPhysicsActivated))

(event Custom|ED_OnPhysicsDeactivated_Event
  (Default|CallEDonPhysicsDeactivated))

(event Custom|ED_OnTargetReached_Event
  (Default|CallEDonTargetReached))

(event Custom|ED_SecondaryActionProjectile_Event
  (Default|CallEDSecondaryActionProjectile))

(event Custom|ED_OnTargetMissing_Event
  (Default|CallEDonTargetMissing))

(event Custom|ED_IsReplace_Event
  (Default|CallEDIsReplace))

(event Custom|ED_OnStartBringBack_Event
  (Default|CallEDonStartBringBack))

(event Custom|ED_OnPhysicsChanged_Event
  (params (CurrentPhysics :type Boolean))
  (Default|CallEDonPhysicsChanged CurrentPhysics))

(event EventTick
  (params (DeltaSeconds :type Float%20%28single-precision%29))
  (bind _bpc_actorphysicsmovement (Variables|Default|GetBPC_ActorPhysicsMovement))
  (bind _ownrootphysics (Variables|/Game/Blueprints/AddOn/Components/BPC_ActorPhysicsMovement.BPC_ActorPhysicsMovement_C|GetOwnRootPhysics _bpc_actorphysicsmovement))
  (Utilities|FlowControl|Sequence
    (:then_0
      (if (Variables|Time|TriggerTime|GetIsTwoTimeProjectile)
        (if (not (Variables|Time|LifeTime|GetbActiveProjectile))
          (if (CallFunction|TimerPos (Variables|Time|TriggerTime|GetTriggerTimeCurrent) (Variables|Time|TriggerTime|GetTriggerTimeMax) 1.0 false)
            (Utilities|FlowControl|DoOnce true
              (:Completed
                (CallFunction|EDActiveProjectileEvent)))))))
    (:then_1
      (if (Variables|Time|LifeTime|GetCanBeDestroy)
        (if (CallFunction|TimerPos (Variables|Time|LifeTime|GetCurrentLifeTime) (Variables|Time|LifeTime|GetLifeTimeMax) 1.0 false)
          (Actor|DestroyActor))))
    (:then_2
      (Utilities|IsValid (Actor|GetAttachParentActor)
        (:Is%20Not%20Valid
          (if (Physics|IsSimulatingPhysics _ownrootphysics "None")
            (Variables|/Game/Blueprints/AddOn/Components/BPC_ActorPhysicsMovement.BPC_ActorPhysicsMovement_C|SetTargetDirection _bpc_actorphysicsmovement (Math|Vector|Normalize (CallFunction|GetVelocity _ownrootphysics)))
            (Default|ApplyRotation _bpc_actorphysicsmovement)))))))

(event EventDestroyed
  (EventDispatchers|UnbindallEventsfromEDActiveProjectileEffect)
  (EventDispatchers|UnbindallEventsfromEDSecondaryActionProjectile)
  (EventDispatchers|UnbindallEventsfromOnDestroyed))

(fn ConstructionScript)

(fn Initialize
  (params (SizeMultiplier :type Float%20%28single-precision%29) (PowerMultiplier :type Float%20%28double-precision%29) (NewLifeTime :type Float%20%28double-precision%29) (NewTriggerTime :type Float%20%28double-precision%29) (ToolThreadParent :type BPC%20Tool%20Thread%20Object%20Reference))
  (Public|ModifyStat|ChangeFloatStatbyMultiplier (Variables|Stat|GetPower) PowerMultiplier)
  (Public|ModifyStat|ChangeSizeEffect SizeMultiplier)
  (Public|ModifyStat|ChangeFloatStat (Variables|Time|LifeTime|GetLifeTimeMax) NewLifeTime)
  (Public|ModifyStat|ChangeFloatStat (Variables|Time|TriggerTime|GetTriggerTimeMax) NewTriggerTime)
  (Variables|Default|SetTool%20Thread%20Parent ToolThreadParent))

(fn ChangeSizeEffect
  (params (SizeMultiplier :type Float%20%28double-precision%29)))

(fn ChangeFloatStatbyMultiplier
  (params (RefValue :type Float%20%28double-precision%29%20%28by%20ref%29) (Multiplier :type Float%20%28double-precision%29))
  (Public|ModifyStat|ChangeFloatStat RefValue (* RefValue Multiplier)))

(fn ChangeFloatStat
  (params (RefValue :type Float%20%28double-precision%29%20%28by%20ref%29) (NewStat :type Float%20%28double-precision%29))
  (|SetBy-RefVar RefValue NewStat))

(fn SetTargetReached
  (params (TargetReached :type Boolean))
  (LocalVariables|SetPreviousValue (Variables|Default|GetTargetReached))
  (Variables|Default|SetTargetReached TargetReached)
  (if (!= (Variables|Default|GetTargetReached) (LocalVariables|GetPreviousValue))
    (if (Variables|Default|GetTargetReached)
      (CallFunction|EDonTargetReachedEvent)
      (else
        (CallFunction|EDonTargetMissingEvent :!label _label)))
    (elif (Variables|Default|GetLaunched)
      (if (not (Variables|Default|GetTargetReached))
        (goto _label)))))

(fn SetLaunched
  (params (IsLaunched :type Boolean))
  (LocalVariables|SetPreviousValue (Variables|Default|GetLaunched))
  (Variables|Default|SetLaunched IsLaunched)
  (if (!= (Variables|Default|GetLaunched) (LocalVariables|GetPreviousValue))
    (if (Variables|Default|GetLaunched)
      (CallFunction|EDonLaunchedEvent)
      (else
        (CallFunction|EDIsReplaceEvent)))))

(fn SetSimulatePhysics
  (params (SimulatePhysics :type Boolean))
  (LocalVariables|SetPreviousValue (Physics|IsSimulatingPhysics (Variables|Default|GetRootCollider) "None"))
  (if (not (== (LocalVariables|GetPreviousValue) SimulatePhysics))
    (Physics|SetSimulatePhysics (Variables|Default|GetRootCollider) SimulatePhysics)
    (CallFunction|EDonPhysicsChangedEvent SimulatePhysics)
    (if SimulatePhysics
      (CallFunction|EDonPhysicsActivatedEvent)
      (else
        (CallFunction|EDonPhysicsDeactivatedEvent)))))