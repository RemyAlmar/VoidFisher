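; Player tool actor that fires a roped sucker projectile, delegating the thread logic to BPC_ToolThread.
; Initialize hands that component the projectile, upgrade data, rope, launch transform and physics constraint.
; A storage box stores the projectile on overlap, with overlaps disabled at launch and re-enabled once the target is reached.
; The construction script lays out mesh and attach points from variables, while component events drive shoot effects and rope-tension audio.
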(event OnComponentBeginOverlap(StorageArea)
  (params (OverlappedComponent :type Primitive%20Component%20Object%20Reference) (OtherActor :type Actor%20Object%20Reference) (OtherComp :type Primitive%20Component%20Object%20Reference) (OtherBodyIndex :type Integer) (bFromSweep :type Boolean) (SweepResult :type Hit%20Result%20Structure%20%28by%20ref%29))
  (if (== OtherActor (Variables|/Game/Blueprints/Game/Player/ToolsComponent/BPC_ToolThread.BPC_ToolThread_C|GetObject (Variables|Default|GetBPC_ToolThread)))
    (Default|CallEDonStoreTool (Variables|Default|GetBPC_ToolThread))))

(event EDonUnlockTool(BPC_ToolThread)
  (bind _object (Variables|/Game/Blueprints/Game/Player/ToolsComponent/BPC_ToolThread.BPC_ToolThread_C|GetObject (Variables|Default|GetBPC_ToolThread))
    (:then
      (EventDispatchers|BindEventtoEDonTargetReached _object (EventDispatchers|CreateEvent :!event Custom|ED_BPC_Object_OnTargetReached_Event))
      (EventDispatchers|BindEventtoEDonLaunched _object (EventDispatchers|CreateEvent :!event Custom|ED_BPC_Object_OnLaunched_Event)))
    (:else)))

(event EDStartTension(BPC_ToolThread)
  (bind _returnvalue (Audio|CreateSound2D "/Game/SFX/Sounds/NEW_OGG/Ventouse/SFX_SuckerRopeStress_Cue.SFX_SuckerRopeStress_Cue" 1.0 1.0 0.0 0))
  (bind _output_get (Variables|Default|SetSFX_CableTaut _returnvalue))
  (Audio|Components|Audio|Play _output_get 0.0))

(event EDEndTension(BPC_ToolThread)
  (bind _sfx_cabletaut (Variables|Default|GetSFX_CableTaut)
    (:then
      (Components|DestroyComponent _sfx_cabletaut))
    (:else)))

(event Custom|ED_BPC_Object_OnLaunched_Event
  (bind _storagearea (Variables|Default|GetStorageArea))
  (Variables|/Script/Engine.PrimitiveComponent|SetbGenerateOverlapEvents (Variables|Default|GetStorageArea) false)
  (Niagara|SpawnSystemAttached "/Game/VFX/Niagara/Player/NS_Shoot.NS_Shoot" _storagearea "None" (Variables|/Script/Engine.SceneComponent|GetRelativeLocation _storagearea) "0, 0, 0" "KeepRelativeOffset" true)
  (Audio|PlaySound2D (Variables|Default|GetSFX_SuckerShoot) 1.0 1.0 0.0 0 0))

(event Custom|ED_BPC_Object_OnTargetReached_Event
  (Variables|/Script/Engine.PrimitiveComponent|SetbGenerateOverlapEvents (Variables|Default|GetStorageArea) true))

(fn ConstructionScript
  (bind _storagearea (Variables|Default|GetStorageArea))
  (Components|SkeletalMesh|SetSkeletalMeshAsset (Variables|Default|GetSkeletalMesh) (Variables|Rendering|GetSM_ToolObject))
  ;[0 1 0.2035] Change Start Cable Location
  (Transformation|SetRelativeLocation (Variables|Default|GetRope_AttachStart) (Variables|LauncherSettings|Rope|GetAttachStartLocation) false false)
  (Transformation|SetRelativeLocation (Variables|Default|GetRope) (Variables|/Script/Engine.SceneComponent|GetRelativeLocation (Variables|Default|GetRope_AttachStart)) false false)
  ;[0 1 0.2035 1 15] Change Launch Transform And Size Area to Bringback the projectile
  (Transformation|SetRelativeTransform (Variables|Default|GetRope_LaunchTransform_Arrow) (Variables|LauncherSettings|Rope|GetLaunchTransform) false false)
  (Components|Box|SetBoxExtent _storagearea (Variables|LauncherSettings|StorageArea|GetAreaSize) true)
  (Transformation|SetRelativeLocation _storagearea (Variables|LauncherSettings|StorageArea|GetAreaLocation) false false)
  (Transformation|SetRelativeLocation (Variables|Default|GetConstr_Location) (Variables|LauncherSettings|Constraint|GetRootConstraintLocation) false false))

(fn Initialize
  (params (RootPossessor :type Primitive%20Component%20Object%20Reference))
  (bind _bpc_toolthread (Variables|Default|GetBPC_ToolThread))
  (Variables|Default|SetRootActor_RootComponent RootPossessor)
  (Variables|/Game/Blueprints/Game/Player/ToolsComponent/BPC_ToolThread.BPC_ToolThread_C|SetObjectToSpawn _bpc_toolthread (Variables|LauncherSettings|Projectile|GetProjectile))
  (Variables|/Game/Blueprints/Game/Player/ToolsComponent/BPC_ToolBase.BPC_ToolBase_C|SetS_Upgrading _bpc_toolthread (Variables|LauncherSettings|Projectile|GetDT_Upgrading))
  (Default|Initialization _bpc_toolthread (Variables|Default|GetRope_LaunchTransform_Arrow) (Variables|Default|GetRope) (Variables|Default|GetPhysicsConstraint) (Variables|Default|GetRootActor_RootComponent) (Variables|LauncherSettings|Stats|GetBaseStatTools) (Variables|Default|GetConstr_Location)))