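; BP_TutoEvent is a tutorial event manager that places tutorial triggers once all creatures are caught.
; It keeps the GameInstance's Spaceport overlap disabled from BeginPlay until a second after that catch event.
; It then re-enables the overlap and spawns BP_TutoCollider actors at the player (hidden, smaller) and at the Spaceport (larger).
; The construction script maps enum keys to DataTuto row names, giving each collider its data row handle.
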(event EventOnAllCreatureCatched
  (bind _gameinstance (Variables|Default|GetGameInstance))
  (bind _spaceport (Variables|/Game/Blueprints/Data/BP_GameInstance.BP_GameInstance_C|GetSpaceport _gameinstance))
  (|CallParentFunction)
  (Utilities|FlowControl|Delay 1.0)
  (Game|SpawnActorfromClass "/Game/Blueprints/Onboarding/BP_TutoCollider.BP_TutoCollider_C" (Transformation|GetActorTransform (Variables|/Game/Blueprints/Data/BP_GameInstance.BP_GameInstance_C|GetPlayer (Variables|Default|GetGameInstance))) "Undefined" "MultiplyWithRoot" 0 false 5e+02 (CallFunction|GetData "NewEnumerator3") 4e+04 "5000.000000,5000.000000,5000.000000" "NewEnumerator1" true 0)
  (Default|ActiveOverlap _spaceport true)
  (Game|SpawnActorfromClass "/Game/Blueprints/Onboarding/BP_TutoCollider.BP_TutoCollider_C" (Transformation|GetActorTransform _spaceport) "Undefined" "MultiplyWithRoot" 0 true 7e+03 (CallFunction|GetData "NewEnumerator4") 4e+04 "5000.000000,5000.000000,5000.000000" "NewEnumerator1" false 0))

(event EventBeginPlay
  (|CallParentFunction)
  (bind _spaceport (Variables|/Game/Blueprints/Data/BP_GameInstance.BP_GameInstance_C|GetSpaceport (Variables|Default|GetGameInstance))
    (:then
      (Default|ActiveOverlap _spaceport false))
    (:else
      (Development|PrintText "Spaceport in Game instance not valid (Manager Event)"))))

(fn ConstructionScript
  (CallFunction|SetDataTable)
  (|CallParentFunction))

(fn SetDataTable
  (bind _datatuto (Variables|Default|GetDataTuto))
  (bind _outrownames (DataTable|GetDataTableRowNames _datatuto))
  (for _array_element _outrownames
    (bind _returnvalue (Utilities|GetDataTableRow _datatuto _array_element)
      (:then
        (Utilities|Map|Add (Variables|Default|GetListRowName) (.KeyEnum (Utilities|Struct|BreakS_TutoriaIInfo _returnvalue)) _array_element))))
  (return))

(fn GetData
  (params (Key :type E_Tuto%20Enum :default "NewEnumerator0"))
  (bind _output_get (LocalVariables|SetLocalData (Utilities|Struct|MakeDataTableRowHandle (Variables|Default|GetDataTuto) (.Value (Utilities|Map|Find (Variables|Default|GetListRowName) Key)))))
  (return _output_get))