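; BP_Medusa is a catchable mini-challenge creature that the player collects by overlapping it.
; When BP_PlayerRefonte overlaps it while its Jiggly mesh is visible, it plays a reward Niagara effect and capture sound, deactivates and calls the OnCatched dispatcher.
; SetActive toggles mesh visibility and actor collision together, so visibility doubles as the catchable state.
; SetMesh allows swapping the mesh and scale.
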(event EventICatched
  (params (Niagara :type Niagara%20System%20Object%20Reference))
  (Niagara|SpawnSystematLocation Niagara (Transformation|GetActorLocation))
  (Audio|SpawnSoundatLocation "/Game/SFX/Sounds/NEW_OGG/Menu_UI_UX/In_Game/SFX_FirstCapture_Cue.SFX_FirstCapture_Cue" (Transformation|GetActorLocation) "0, 0, 0" 2.0 1.0 0.0 0 0)
  (CallFunction|SetActive false)
  (Default|CallEDonCatched))

(event Collision|EventActorBeginOverlap
  (params (OtherActor :type Actor%20Object%20Reference))
  (if (== (Utilities|GetClass OtherActor) "/Game/Blueprints/Game/Player/Controllers/BP_PlayerRefonte.BP_PlayerRefonte_C")
    (bind _iscatcheable (CallFunction|IIsCatcheable))
    (if _iscatcheable
      (CallFunction|ICatched "/Game/VFX/Niagara/Environment/Chall/NS_ChallGetReward.NS_ChallGetReward"))))

(fn ConstructionScript)

(fn SetActive
  (params (isActive :type Boolean))
  (Rendering|SetVisibility (Variables|Default|GetJiggly) isActive false)
  (Collision|SetActorEnableCollision isActive))

(fn SetMesh
  (params (NewMesh :type Static%20Mesh%20Object%20Reference) (NewScale :type Vector))
  (bind _jiggly (Variables|Default|GetJiggly))
  (Components|StaticMesh|SetStaticMesh _jiggly NewMesh)
  (Transformation|SetWorldScale3D _jiggly NewScale))

(fn IGetCreatureData
  (return ""))

(fn IIsCatcheable
  (return (Rendering|IsVisible (Variables|Default|GetJiggly))))