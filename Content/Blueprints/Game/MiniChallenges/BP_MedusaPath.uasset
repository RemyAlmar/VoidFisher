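; Timed mini-challenge where the player collects jellyfish (BP_Medusa) spawned at even spacing along a spline.
; Entering the start collider fades, repositions the player and runs a countdown widget before enabling the timer and end trigger.
; Timeout or reaching the end succeeds with 90% caught; catching all wins immediately.
; Success triggers rewards and destroys the challenge; failure resets it and teleports the player to a respawn point.
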(event OnComponentBeginOverlap(ActivationCollider)
  (params (OverlappedComponent :type Primitive%20Component%20Object%20Reference) (OtherActor :type Actor%20Object%20Reference) (OtherComp :type Primitive%20Component%20Object%20Reference) (OtherBodyIndex :type Integer) (bFromSweep :type Boolean) (SweepResult :type Hit%20Result%20Structure%20%28by%20ref%29))
  (bind _player (Variables|Default|GetPlayer))
  (bind _activationcollider (Variables|Default|GetActivationCollider))
  (bind _returnvalue (Transformation|GetWorldTransform _activationcollider))
  (if (== OtherActor (Variables|Default|GetPlayer))
    (Audio|PlaySound2D "/Game/SFX/Sounds/NEW_OGG/Enviro/Challenge/SFX_ChallengeAccepted_Cue.SFX_ChallengeAccepted_Cue" 1.0 1.0 0.0 0 0)
    (CallFunction|ActivationVisibility)
    (Default|FadeinFadeOut (Variables|Default|GetFade) 2.0 5.0)
    (Default|StopInput _player)
    (Default|CallEDPlayerinChall _player)
    (Utilities|FlowControl|Delay 1.0)
    (Transformation|SetActorLocationAndRotation (Variables|Default|GetPlayer) (.location _returnvalue) (.rotation _returnvalue) false true)
    (Utilities|FlowControl|Delay 2.0)
    (Default|Start (Variables|Widget|GetWidgetCount))))

(event OnComponentBeginOverlap(EndChall)
  (params (OverlappedComponent :type Primitive%20Component%20Object%20Reference) (OtherActor :type Actor%20Object%20Reference) (OtherComp :type Primitive%20Component%20Object%20Reference) (OtherBodyIndex :type Integer) (bFromSweep :type Boolean) (SweepResult :type Hit%20Result%20Structure%20%28by%20ref%29))
  (if (== OtherActor (Variables|Default|GetPlayer))
    (CallFunction|OnChallengeTimeFinishedEvent)))

(event Custom|ActivationChallenge
  (bind _returnvalue (Audio|SpawnSound2D "/Game/SFX/Sounds/NEW_OGG/Enviro/Challenge/SFX_ClockChallenge_Cue.SFX_ClockChallenge_Cue" 1.0 1.0 0.0 0 false false))
  (Variables|Sound|SetChronoSound _returnvalue)
  (CallFunction|ActivationFlowNS true)
  (CallFunction|ActiveComponent (Variables|Default|GetEndChall) true))

(event Custom|ChallengeCompleted
  (bind _returnvalue (Game|Player|GetPlayerPawn 0))
  (bind _returnvalue_2 (Transformation|GetActorLocation _returnvalue))
  (Variables|Challenge|SetChallengeActivated false)
  (Niagara|SpawnSystematLocation "/Game/VFX/Niagara/Player/NS_FireworkUpgradeTool.NS_FireworkUpgradeTool" _returnvalue_2 (Transformation|GetActorRotation _returnvalue) "1.000000,1.000000,1.000000" false)
  (Audio|SpawnSoundatLocation "/Game/SFX/Sounds/NEW_OGG/Enviro/Challenge/SFX_ChallengeWin_Cue.SFX_ChallengeWin_Cue" _returnvalue_2 "0, 0, 0" 1.0 1.0 0.0 0 0)
  (Default|AnimationCompleted (Variables|Widget|GetWidgetCount))
  (Audio|Components|Audio|Stop (Variables|Sound|GetChronoSound))
  (Default|CallEDonChallengeCompleted self)
  (CallFunction|OnChallengeDone))

(event Custom|ChallengeFailed
  (bind _respawnfailed (Variables|Default|GetRespawnFailed))
  (bind _returnvalue (Transformation|GetWorldTransform _respawnfailed))
  (Variables|Challenge|SetChallengeActivated false)
  (CallFunction|ResetChallenge)
  (Audio|Components|Audio|Stop (Variables|Sound|GetChronoSound))
  (Audio|SpawnSound2D "/Game/SFX/Sounds/NEW_OGG/Enviro/Challenge/SFX_ChallengeLost_Cue.SFX_ChallengeLost_Cue" 1.0 1.0 0.0 0)
  (Class|NiagaraComponent|SetRenderingEnabled (Variables|Default|GetNS_ChallActive) true)
  (Default|CallEDonChallengeFailed self)
  (Utilities|FlowControl|Delay 2.0)
  (Default|StopInput (Variables|Default|GetPlayer))
  (Default|FadeinFadeOut (Variables|Default|GetFade) 2.0 5.0)
  (Utilities|FlowControl|Delay 1.0)
  (Transformation|SetActorLocationAndRotation (Variables|Default|GetPlayer) (.location _returnvalue) (.rotation _returnvalue) false true)
  (Default|ActiveInput (Variables|Default|GetPlayer)))

(event Custom|OnChallengeTimeFinished_Event
  (Default|CallEDPlayerOutChall (Variables|Default|GetPlayer))
  (Components|DestroyComponent (Variables|Default|GetNS_EndStar))
  (if (>= (Variables|Objects|GetObjectCatched) (Variables|Objects|GetObjectsNeeded))
    (CallFunction|ChallengeCompleted)
    (else
      (CallFunction|ChallengeFailed))))

(event Custom|OnChallengeDone
  (CallFunction|DestroyObjects)
  (CallFunction|DoAspectAllRewards)
  (Actor|DestroyActor))

(event Custom|ActivationVisibility
  (Widget|SetVisibility (Variables|Widget|GetWidgetCount) "HitTestInvisible")
  (Default|SetTimer (Variables|Widget|GetWidgetCount) (Variables|Challenge|GetMaxTime) (Variables|Challenge|GetCurrentTime))
  (CallFunction|ActiveAllObjectstoCatch true) ; Active les objets à recuperer
  (Class|NiagaraComponent|SetRenderingEnabled (Variables|Default|GetNS_ChallActive) false)
  (CallFunction|ActiveComponent (Variables|Default|GetActivationCollider) false) ; Desactive le collider d'activation
  (Default|SetTimer (Variables|Widget|GetWidgetCount) (Variables|Challenge|GetMaxTime) (Variables|Challenge|GetCurrentTime)))

(event Custom|ED_CanStart
  (CallFunction|ActivationChallenge)
  (Default|ActiveInput (Variables|Default|GetPlayer))
  (Variables|Challenge|SetChallengeActivated true)
  (bind _returnvalue (Niagara|SpawnSystemAttached "/Game/VFX/Niagara/Environment/Chall/NS_ChallengeEnd.NS_ChallengeEnd" (Variables|Default|GetEndChall) "None" "0, 0, 0" "0, 0, 0" "KeepRelativeOffset" false))
  (Variables|Default|SetNS_EndStar _returnvalue))

(event EventBeginPlay
  (bind _sm_challdebug (Variables|Default|GetSM_ChallDebug))
  ;[0.2104 0.8902 1] Initialize en créant les objets à recuperer
  (|CallParentFunction)
  (Variables|Challenge|SetCurrentTime (Variables|Challenge|GetMaxTime))
  (Variables|Objects|SetObjectsNeeded (Math|Float|Truncate (* (Variables|Objects|GetTotalNumberObject) 0.9)))
  (Utilities|Array|Clear (Variables|Objects|GetObjectToCatch))
  (CallFunction|SetObjectsinSpline)
  (CallFunction|AddWidget)
  (Rendering|SetVisibility _sm_challdebug false false) ; Debug
  (bind _returnvalue (Niagara|SpawnSystemAttached "/Game/VFX/Niagara/Environment/Chall/NS_ChallengeStar.NS_ChallengeStar" _sm_challdebug "None" "0, 0, 0" "0, 0, 0" "KeepRelativeOffset" false))
  (Variables|Default|SetNS_ChallActive _returnvalue)
  (EventDispatchers|BindEventtoCanStart (Variables|Widget|GetWidgetCount) (EventDispatchers|CreateEvent :!event Custom|ED_CanStart))
  (CallFunction|ActiveComponent (Variables|Default|GetEndChall) false)
  (bind _returnvalue_2 (UserInterface|CreateWidget "/Game/Sequence/UI/UI_FadeToDarknesse.UI_FadeToDarknesse_C"))
  (UserInterface|Viewport|AddtoViewport _returnvalue_2 200)
  (Variables|Default|SetFade _returnvalue_2))

(event EventTick
  (params (DeltaSeconds :type Float%20%28single-precision%29))
  (|CallParentFunction DeltaSeconds)
  (if (Variables|Challenge|GetChallengeActivated)
    (if (CallFunction|TimerNeg (Variables|Challenge|GetCurrentTime) (Variables|Challenge|GetMaxTime) 1.0 true)
      (CallFunction|OnChallengeTimeFinishedEvent)
      (else
        (Default|SetTimer (Variables|Widget|GetWidgetCount) (Variables|Challenge|GetMaxTime) (Variables|Challenge|GetCurrentTime))))))

(fn ConstructionScript
  (bind (_location _tangent _rotation) (CallFunction|GetLastPointLocation))
  (|CallParentFunction)
  (Transformation|SetRelativeTransform (Variables|Default|GetEndChall) (Math|Transform|MakeTransform (+ (* (Math|Vector|GetForwardVector _rotation) 5e+02) _location) _rotation) false true))

(fn ActivationFlowNS
  (params (IsActive :type Boolean))
  (Class|NiagaraComponent|SetRenderingEnabled (Variables|Default|GetNiagara) IsActive))

(fn ActiveAllObjectstoCatch
  (params (isActive :type Boolean))
  (Variables|Default|SetEnable isActive) ; Active le flow
  (for _array_element (Variables|Objects|GetObjectToCatch)
    (Default|SetActive _array_element isActive)))

(fn ActiveComponent
  (params (Component :type Primitive%20Component%20Object%20Reference) (bNewActive :type Boolean))
  (Components|Activation|SetActive Component bNewActive false)
  (Rendering|SetVisibility Component bNewActive true)
  (if bNewActive
    (Collision|SetCollisionEnabled Component "QueryAndPhysics")
    (else
      (Collision|SetCollisionEnabled Component "NoCollision"))))

(fn OnObjectCatched
  (bind _result (Math|Integer|IncrementInt (Variables|Objects|GetObjectCatched))
    (:%20%20
      (Default|UpdateMedusa (Variables|Widget|GetWidgetCount) _result)
      (if (>= (Variables|Objects|GetObjectCatched) (Variables|Objects|GetTotalNumberObject))
        (CallFunction|ChallengeCompleted)))))

(fn ResetChallenge
  (CallFunction|ActiveAllObjectstoCatch false)
  (CallFunction|ActiveComponent (Variables|Default|GetActivationCollider) true)
  (Variables|Objects|SetObjectCatched 0)
  (Widget|SetVisibility (Variables|Widget|GetWidgetCount) "Hidden")
  (CallFunction|ActivationFlowNS false)
  (CallFunction|ActiveComponent (Variables|Default|GetEndChall) false))

(fn DestroyObjects
  (for _array_element (Variables|Objects|GetObjectToCatch)
    (Actor|DestroyActor _array_element)))

(fn SetObjectsinSpline
  (bind _spline (Variables|Default|GetSpline))
  (for _index (range 0 (- (Variables|Objects|GetTotalNumberObject) 1))
    (bind _returnvalue (Game|SpawnActorfromClass "/Game/Blueprints/Game/MiniChallenges/BP_Medusa.BP_Medusa_C" (Math|Transform|MakeTransform (Spline|GetLocationatDistanceAlongSpline _spline (* _index (Variables|Construct|GetSpacing)) "World") (Spline|GetRotationatDistanceAlongSpline _spline (* _index (Variables|Construct|GetSpacing)) "World")) "AlwaysSpawn" "MultiplyWithRoot" 0 0))
    (Default|SetActive _returnvalue false)
    (EventDispatchers|BindEventtoEDonCatched _returnvalue (EventDispatchers|CreateEvent :!event OnObjectCatched))
    (Utilities|Array|Add (Variables|Objects|GetObjectToCatch) _returnvalue) ; On enregistre toutes les méduses de ce spawner
    (Default|SetMesh _returnvalue (Variables|Debug|GetPointsMesh) (Variables|Debug|GetScalePoints))))

(fn AddWidget
  (bind _returnvalue (UserInterface|CreateWidget "/Game/Blueprints/Widgets/MainShipHUD/UI_CountMedusa.UI_CountMedusa_C" 0 (Variables|Objects|GetObjectsNeeded)))
  (UserInterface|Viewport|AddtoViewport _returnvalue 0)
  (bind _output_get (Variables|Widget|SetWidgetCount _returnvalue))
  (Widget|SetVisibility _output_get "Collapsed"))

(fn DoAspectAllRewards
  (bind _objectreward (Variables|Objects|GetObjectReward))
  (for _array_element _objectreward
    (Class|BPICollecteable|IonAspect(Message) _array_element))
  (Default|NewCameraView (Variables|Default|GetPlayer) (Utilities|Array|Get(acopy) _objectreward (Utilities|Array|LastIndex _objectreward)) 3.0)
  (return))

(fn DoDisappearsAllRewards
  (for _array_element (Variables|Objects|GetObjectReward)
    (Class|BPICollecteable|IonDisappears(Message) _array_element))
  (return))

(fn GetLastPointLocation
  (bind _spline (Variables|Default|GetSpline))
  (bind _returnvalue (Spline|GetNumberOfSplinePoints _spline))
  (bind _returnvalue_2 (- _returnvalue 1))
  (bind _returnvalue_3 (Spline|GetSplinePointAt _spline _returnvalue_2 "Local"))
  (return (.position _returnvalue_3) (.arrivetangent _returnvalue_3) (.rotation _returnvalue_3)))