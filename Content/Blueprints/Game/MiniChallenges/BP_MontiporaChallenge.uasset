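; Manager actor for the Montipora mini-challenge, coordinating the BP_MedusaPath actors in the level.
; After a short BeginPlay delay that lets paths spawn, it gathers every path, registers itself as their manager, then caches the game instance.
; ChallengeComplete clears CanChallenge on the given path if it is one of those gathered, disabling that path's challenge.
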(event EventBeginPlay
  (Utilities|FlowControl|Delay 0.2) ; On laisse le temps au medusa path de s'instancier
  (CallFunction|Initialise)
  (bind _asbp_game_instance (Utilities|Casting|CastToBP_GameInstance (Game|GetGameInstance)))
  (Variables|Default|SetBP%20Game%20Instance _asbp_game_instance))

(fn ConstructionScript)

(fn Initialise
  (bind _outactors (Actor|GetAllActorsOfClass "/Game/Blueprints/Game/MiniChallenges/BP_MedusaPath.BP_MedusaPath_C"))
  (bind _output_get (Variables|Default|SetMedusa%20Path _outactors))
  (for _array_element _output_get
    (Default|SetManager _array_element self)))

(fn ChallengeComplete
  (params (ItemToFind :type BP%20Medusa%20Path%20Object%20Reference%20%28by%20ref%29))
  (if (Utilities|Array|ContainsItem (Variables|Default|GetMedusa%20Path) ItemToFind)
    (Variables|/Game/Blueprints/Game/MiniChallenges/BP_MedusaPath.BP_MedusaPath_C|SetCanChallenge ItemToFind false)))

(fn GameInstance
  (bind _bp_game_instance (Variables|Default|GetBP%20Game%20Instance)
    (:then
      (return _bp_game_instance))
    (:else)))