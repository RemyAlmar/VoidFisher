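; BP_TutoEvent is a tutorial event that gates the spaceport until all creatures are caught.
; It disables spaceport overlap at start, then shortly after the catch completes re-enables it and opens an optional linked door.
; It also spawns tutorial collider managers at the player and the spaceport, passing the latter a tutorial data row.
; Construction maps DataTuto row names by enum key for that lookup.
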(event EventOnAllCreatureCatched
  (bind _gameinstance (CallFunction|GetBPGameInstance))
  (bind _door_to_open (Variables|Default|GetDoor%20To%20open))
  (bind _spaceport (Default|GetSpaceport _gameinstance))
  (bind _returnvalue (Transformation|GetActorTransform _spaceport))
  (|CallParentFunction)
  (Utilities|FlowControl|Delay 1.0)
  (Game|SpawnActorfromClass :Class "/Game/Blueprints/Onboarding/BP_TutoColliderManager.BP_TutoColliderManager_C" :SpawnTransform (Transformation|GetActorTransform (Default|GetPlayer (CallFunction|GetBPGameInstance))) :CollisionHandlingOverride "Undefined" :TransformScaleMethod "MultiplyWithRoot" :BeginOverlap false :Radius 5e+02 :Shape "NewEnumerator1" :Hidden%20in%20Game true :Instigator 0)
  (Default|ActiveOverlap _spaceport true)
  (Game|SpawnActorfromClass "/Game/Blueprints/Onboarding/BP_TutoColliderManager.BP_TutoColliderManager_C" (Math|Transform|MakeTransform (.location _returnvalue) (.rotation _returnvalue) "1.000000,1.000000,1.000000") "Undefined" "MultiplyWithRoot" 0 true 5.2e+03 (CallFunction|GetData "NewEnumerator4") 4e+04 "6000.000000,2500.000000,2500.000000" "NewEnumerator2" false 0)
  (Utilities|IsValid _door_to_open
    (:Is%20Valid
      (Default|CallEDOpenDoor _door_to_open))))

(event EventBeginPlay
  (|CallParentFunction)
  (Default|ActiveOverlap (Default|GetSpaceport (CallFunction|GetBPGameInstance)) false))

(fn ConstructionScript
  (CallFunction|SetDataTable)
  (|CallParentFunction))

(fn SetDataTable
  (bind _datatuto (Variables|Default|GetDataTuto))
  (bind _outrownames (DataTable|GetDataTableRowNames _datatuto))
  (for _array_element _outrownames
    (bind _returnvalue (Utilities|GetDataTableRow _datatuto _array_element)
      (:then
        (Utilities|Map|Add (Variables|Default|GetListRowName) (.KeyEnum (Utilities|Struct|BreakS_TutoriaIInfo _returnvalue)) _array_element))))
  (return))

(fn GetData
  (params (Key :type E_Tuto%20Enum :default "NewEnumerator0"))
  (bind _output_get (LocalVariables|SetLocalData (Utilities|Struct|MakeDataTableRowHandle (Variables|Default|GetDataTuto) (.Value (Utilities|Map|Find (Variables|Default|GetListRowName) Key)))))
  (return _output_get))