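; BP_LimitArea is a boundary volume, shaped as a configurable sphere, capsule or box, that steers departing physics-moved actors back inside.
; Actors with BPC_ActorPhysicsMovement that leave are listed as out, and re-entries are also listed as in.
; While ticking, it sets each out actor's target direction and pushing force toward the volume's center.
; An actor is released once back inside and facing the center, or when destroyed.
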(event Custom|OnEndOverlap
  (params (OverlappedComponent :type Primitive%20Component%20Object%20Reference) (OtherActor :type Actor%20Object%20Reference) (OtherComp :type Primitive%20Component%20Object%20Reference) (OtherBodyIndex :type Integer))
  (Utilities|IsValid (Actor|GetComponentbyClass OtherActor "/Game/Blueprints/AddOn/Components/BPC_ActorPhysicsMovement.BPC_ActorPhysicsMovement_C")
    (:Is%20Valid
      (Game|BindEventtoOnDestroyed OtherActor (EventDispatchers|CreateEvent :!event Custom|ActorDestroyed))
      (Utilities|Array|AddUnique (Variables|Default|GetListActorOut) OtherActor))
    (:Is%20Not%20Valid
      _))
  (Actor|Tick|SetActorTickEnabled (Utilities|Array|IsNotEmpty (Variables|Default|GetListActorOut))))

(event Custom|OnBeginOverlap
  (params (OverlappedComponent :type Primitive%20Component%20Object%20Reference) (OtherActor :type Actor%20Object%20Reference) (OtherComp :type Primitive%20Component%20Object%20Reference) (OtherBodyIndex :type Integer) (bFromSweep :type Boolean) (SweepResult :type Hit%20Result%20Structure%20%28by%20ref%29))
  (if (Utilities|Array|ContainsItem (Variables|Default|GetListActorOut) OtherActor)
    (Utilities|Array|AddUnique (Variables|Default|GetListActorIn) OtherActor)))

(event Custom|ActorDestroyed
  (params (DestroyedActor :type Actor%20Object%20Reference))
  (bind _listactorout (Variables|Default|GetListActorOut))
  (if (Utilities|Array|ContainsItem _listactorout DestroyedActor)
    (Utilities|Array|RemoveItem _listactorout DestroyedActor)
    (Utilities|Array|RemoveItem (Variables|Default|GetListActorIn) DestroyedActor)))

(event EventTick
  (params (DeltaSeconds :type Float%20%28single-precision%29))
  (CallFunction|BringActorsinShere))

(fn ConstructionScript
  (bind _radius (Variables|Param|Shape|Radius|GetRadius))
  (bind _capsule (Variables|Default|GetCapsule))
  (Components|Sphere|SetSphereRadius (Variables|Default|GetSphere) _radius true)
  (Components|Capsule|SetCapsuleRadius _capsule _radius true)
  (Components|Capsule|SetCapsuleHalfHeight _capsule (Variables|Param|Shape|Capsule|GetCapsuleHeight) true)
  (Components|Box|SetBoxExtent (Variables|Default|GetBox) (Variables|Param|Shape|Box|GetExtent) true)
  (CallFunction|SetShape))

(fn BringActorsinShere
  (for _array_element (Variables|Default|GetListActorOut)
    (Utilities|IsValid _array_element
      (:Is%20Valid
        (bind _output_get (LocalVariables|SetDirectionToGo (CallFunction|GetDirectiontoGo _array_element)))
        (bind _output_get_2 (Variables|/Game/Blueprints/AddOn/Components/BPC_ActorPhysicsMovement.BPC_ActorPhysicsMovement_C|SetTargetDirection (Actor|GetComponentbyClass _array_element "/Game/Blueprints/AddOn/Components/BPC_ActorPhysicsMovement.BPC_ActorPhysicsMovement_C") _output_get))
        (Default|SetOtherForcesMovement (Actor|GetComponentbyClass _array_element "/Game/Blueprints/AddOn/Components/BPC_ActorPhysicsMovement.BPC_ActorPhysicsMovement_C") (* _output_get_2 6e+03))
        (if (and (Utilities|Operators|EqualEqual (Transformation|GetActorForwardVector _array_element) (LocalVariables|GetDirectionToGo) 0.01) (Utilities|Array|ContainsItem (Variables|Default|GetListActorIn) _array_element))
          (Utilities|Array|RemoveItem (Variables|Default|GetListActorOut) _array_element)
          (Utilities|Array|RemoveItem (Variables|Default|GetListActorIn) _array_element)
          (Actor|Tick|SetActorTickEnabled (and (Utilities|Array|IsNotEmpty (Variables|Default|GetListActorOut)) (Utilities|Array|IsNotEmpty (Variables|Default|GetListActorIn))))))))
  (return))

(fn SetShape
  (switch Utilities|FlowControl|Switch|SwitchonE_CollisionShape (Variables|Param|Shape|GetShape)
    (:NewEnumerator1
      (Variables|Default|SetShape%20Collision (Variables|Default|GetSphere)))
    (:NewEnumerator0
      (Variables|Default|SetShape%20Collision (Variables|Default|GetCapsule)))
    (:NewEnumerator2
      (Variables|Default|SetShape%20Collision (Variables|Default|GetBox))))
  (Collision|BindEventtoOnComponentEndOverlap (Variables|Default|GetShape%20Collision) (EventDispatchers|CreateEvent :!event Custom|OnEndOverlap))
  (Collision|BindEventtoOnComponentBeginOverlap (Variables|Default|GetShape%20Collision) (EventDispatchers|CreateEvent :!event Custom|OnBeginOverlap))
  (Rendering|SetVisibility (Variables|Default|GetShape%20Collision) true false)
  (Development|SetHiddeninGame (Variables|Default|GetShape%20Collision) (Variables|Param|GetHiddenInGame) false))

(fn GetDirectiontoGo
  (params (Target :type Actor%20Object%20Reference))
  (return (Math|Vector|GetUnitDirection(Vector) (Transformation|GetActorLocation Target) (Transformation|GetActorLocation))))