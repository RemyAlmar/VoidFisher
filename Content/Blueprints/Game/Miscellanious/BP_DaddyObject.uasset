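; BP_DaddyObject is a collectible artifact actor whose mesh and material come from a data table row.
; Init attaches a Niagara effect and creates a dynamic material with a dissolve parameter.
; Player overlap fires the collected event and sound, then a timeline animates the dissolve before destroying the actor.
; Interface functions store and query its micro area, and toggle visibility, overlap and proximity sound as it appears or disappears.
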(event OnComponentBeginOverlap(Coll_TriggerToCollect)
  (params (OverlappedComponent :type Primitive%20Component%20Object%20Reference) (OtherActor :type Actor%20Object%20Reference) (OtherComp :type Primitive%20Component%20Object%20Reference) (OtherBodyIndex :type Integer) (bFromSweep :type Boolean) (SweepResult :type Hit%20Result%20Structure%20%28by%20ref%29))
  (Utilities|Casting|CastToBP_PlayerRefonte OtherActor)
  (CallFunction|ICollected)
  (Audio|PlaySound2D "/Game/SFX/Sounds/NEW_OGG/Enviro/DaddyObjetcs/SFX_ArtefactFind_Cue.SFX_ArtefactFind_Cue" 1.0 1.0 0.0 0 0)
  (bind _dissolve_alpha (Timeline|Alpha%20Timeline PlayFromStart)
    (:Update
      (Rendering|Material|SetScalarParameterValue (Variables|Default|GetInstancied%20Material) "DissolveMask" _dissolve_alpha :!class /Script/Engine.MaterialInstanceDynamic))
    (:Finished
      (Components|DestroyComponent (Variables|Default|Getniagara))
      (Actor|DestroyActor))))

(event Custom|Init
  (bind _out_row (CallFunction|GetDatafromRow))
  (bind (_objectname _picture _mesh _description _material) (Utilities|Struct|BreakS_DaddyObject _out_row))
  (Variables|Default|SetDataObject _out_row)
  (bind _returnvalue (Niagara|SpawnSystemAttached "/Game/VFX/Niagara/Environment/NS_Artifact.NS_Artifact" (Variables|Default|GetStaticMesh) "None" "0, 0, 0" "0, 0, 0" "KeepRelativeOffset" false))
  (Variables|Default|Setniagara _returnvalue)
  (bind _returnvalue_2 (Rendering|Material|CreateDynamicMaterialInstance (Variables|Default|GetStaticMesh) 0 _material "None" :!class /Script/Engine.PrimitiveComponent))
  (Rendering|Material|SetScalarParameterValue _returnvalue_2 "DissolveMask" 1.0 :!class /Script/Engine.MaterialInstanceDynamic)
  (Variables|Default|SetInstancied%20Material _returnvalue_2)
  (Components|StaticMesh|SetStaticMesh (Variables|Default|GetStaticMesh) _mesh))

(event EventISetMicroArea
  (params (TargetArea :type E_MicroZone%20Enum :default "NewEnumerator4"))
  (bind _output_get (Variables|Default|SetMicro%20Area TargetArea))
  (Variables|Default|SetDataFinal (Utilities|Struct|MakeS_Artifact (Variables|Default|GetDataObject) _output_get)))

(event EventICollected
  (Default|CallEDonCollected self))

(event EventIonAspect
  (Rendering|SetVisibility (Variables|Default|GetStaticMesh) true true)
  (Variables|/Script/Engine.PrimitiveComponent|SetbGenerateOverlapEvents (Variables|Default|GetColl_TriggerToCollect) true)
  (Components|Activation|SetActive (Variables|Default|GetSFXProximity) true false))

(event EventIonDisappears
  (Rendering|SetVisibility (Variables|Default|GetStaticMesh) false true)
  (Variables|/Script/Engine.PrimitiveComponent|SetbGenerateOverlapEvents (Variables|Default|GetColl_TriggerToCollect) false)
  (Components|Activation|SetActive (Variables|Default|GetSFXProximity) false false))

(fn ConstructionScript
  (bind _out_row (CallFunction|GetDatafromRow))
  (Components|StaticMesh|SetStaticMesh (Variables|Default|GetStaticMesh) (.Mesh (Utilities|Struct|BreakS_DaddyObject _out_row)))
  (Variables|Default|SetDataObject _out_row))

(fn GetDatafromRow
  (bind _dataobjectrow (Variables|Data|GetDataObjectRow))
  (bind (_datatable _rowname) (Utilities|Struct|BreakDataTableRowHandle _dataobjectrow))
  (bind _returnvalue (Utilities|GetDataTableRow _datatable _rowname)
    (:then
      (return _returnvalue))))

(fn IGetPriority
  (return 0))

(fn IGetMicroArea
  (return (Variables|Default|GetMicro%20Area)))

(fn IIsinMicroArea
  (params (Target :type E_MicroZone%20Enum :default "NewEnumerator4"))
  (return (Utilities|Enum|Equal(Enum) (Variables|Default|GetMicro%20Area) Target)))