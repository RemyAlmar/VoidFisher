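; BP_AnchorPoint is a spherical anchor that other actors snap and attach to, firing a grab-anchor event dispatcher when they do.
; On attach, it replaces any previous anchor with a visible arrow component on the sphere's radius toward the target, pointing back at the center.
; The target's root primitive stops simulating physics, then teleports to that arrow and attaches.
; SetSize scales collision radius and sphere mesh together from the construction-time base radius.
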(event Custom|ED_OnGrabAnchor_Event)

(event EventIAttachActortoComp
  (params (TargetToAttach :type Actor%20Object%20Reference))
  (bind _anchorpoint (Variables|Default|GetAnchorPoint))
  (CallFunction|AddAnchorPoint TargetToAttach)
  (bind _asprimitive_component (Utilities|Casting|CastToPrimitiveComponent (Variables|/Script/Engine.Actor|GetRootComponent TargetToAttach)))
  (Physics|SetSimulatePhysics _asprimitive_component false)
  (Transformation|SetActorLocationAndRotation TargetToAttach (Transformation|GetWorldLocation _anchorpoint) (Transformation|GetWorldRotation _anchorpoint) false true)
  (Transformation|AttachComponentToComponent TargetToAttach (Variables|Default|GetAnchorPoint) "None" "KeepWorld" "KeepWorld" "KeepWorld" false)
  (Default|CallEDonGrabAnchor))

(fn ConstructionScript
  (EventDispatchers|BindEventtoEDonGrabAnchor (EventDispatchers|CreateEvent :!event Custom|ED_OnGrabAnchor_Event))
  (Variables|Default|SetBaseRadius (Variables|/Script/Engine.SphereComponent|GetSphereRadius (Variables|Default|GetSphere))))

(fn AddAnchorPoint
  (params (TargetActor :type Actor%20Object%20Reference))
  (bind _returnvalue (Transformation|GetActorLocation TargetActor))
  (bind _returnvalue_2 (Transformation|GetActorLocation))
  (bind _returnvalue_3 (Math|Vector|GetUnitDirection(Vector) _returnvalue_2 _returnvalue))
  (bind _anchorpoint (Variables|Default|GetAnchorPoint)
    (:then
      (Components|DestroyComponent _anchorpoint))
    (:else
      _))
  (bind _returnvalue_4 (AddComponent|AddArrowComponent false (Math|Transform|MakeTransform (* _returnvalue_3 (Variables|/Script/Engine.SphereComponent|GetSphereRadius (Variables|Default|GetSphere))) (Math|Conversions|RotationFromXVector (* _returnvalue_3 -1.0)) "1.000000,1.000000,1.000000")))
  (bind _output_get (Variables|Default|SetAnchorPoint _returnvalue_4))
  (Development|SetHiddeninGame _output_get false false)
  (Rendering|SetVisibility _output_get true false)
  (return))

(fn SetSize
  (params (Size :type Float%20%28double-precision%29))
  (bind _baseradius (Variables|Default|GetBaseRadius))
  (bind _returnvalue (* Size _baseradius))
  (Components|Sphere|SetSphereRadius (Variables|Default|GetSphere) _returnvalue true)
  (Transformation|SetWorldScale3D (Variables|Default|GetSM_Sphere) (Math|Conversions|ToVector(Float) (/ _returnvalue 5e+01)))
  (return))