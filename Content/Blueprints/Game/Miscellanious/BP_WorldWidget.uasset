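; BP_WorldWidget is a world widget Blueprint that displays UI supplied through its WidgetToSpawn variable.
; Its construction script passes the widget instance from WidgetToSpawn to its own Widget component and makes that component visible, without propagating visibility to children.
; It also copies the draw size and widget space from WidgetToSpawn, so the display mirrors that source's setup.
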(fn ConstructionScript
  (bind _widget (Variables|Default|GetWidget))
  (bind _widget_2 (Variables|Default|GetWidget))
  (bind _widgettospawn (Variables|Default|GetWidgetToSpawn))
  (UserInterface|SetWidget _widget (UserInterface|GetWidget _widgettospawn))
  (Rendering|SetVisibility _widget true false)
  (Class|WidgetComponent|SetDrawSize _widget_2 (Class|WidgetComponent|GetDrawSize _widgettospawn))
  (Class|WidgetComponent|SetWidgetSpace _widget_2 (Class|WidgetComponent|GetWidgetSpace (Variables|Default|GetWidgetToSpawn))))