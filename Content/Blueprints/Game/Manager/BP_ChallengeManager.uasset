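; BP_ChallengeManager tracks the BP_MedusaPath challenges in the level and restores their completion state from the current save slot.
; On BeginPlay, it gathers every path, binds its completed and failed dispatchers, and registers it in the save by display name.
; Paths already saved as completed receive OnChallengeDone.
; The completion handler unbinds a path and removes it from the tracked list, while the failure handler is empty.
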(event Custom|ED_OnChallengeCompleted_Event
  (params (ChallengeTarget :type BP%20Medusa%20Path%20Object%20Reference))
  (EventDispatchers|UnbindallEventsfromEDonChallengeCompleted ChallengeTarget)
  (EventDispatchers|UnbindallEventsfromEDonChallengeFailed ChallengeTarget)
  (Utilities|Array|RemoveItem (Variables|Default|GetChallengeMedusaPath) ChallengeTarget))

(event Custom|ED_OnChallengeFailed_Event
  (params (ChallengeTarget :type BP%20Medusa%20Path%20Object%20Reference)))

(event EventBeginPlay
  (CallFunction|Initialize))

(fn ConstructionScript
  (|CallParentFunction))

(fn Initialize
  (bind _bpgame_instance (CallFunction|GetBPGameInstance))
  (bind _currentsaveslot (Default|GetCurrentSaveSlot _bpgame_instance))
  (bind _outactors (Actor|GetAllActorsOfClass "/Game/Blueprints/Game/MiniChallenges/BP_MedusaPath.BP_MedusaPath_C"))
  (bind _output_get (Variables|Default|SetChallengeMedusaPath _outactors))
  (for _array_element _output_get
    (EventDispatchers|BindEventtoEDonChallengeCompleted _array_element (EventDispatchers|CreateEvent :!event Custom|ED_OnChallengeCompleted_Event))
    (EventDispatchers|BindEventtoEDonChallengeFailed _array_element (EventDispatchers|CreateEvent :!event Custom|ED_OnChallengeFailed_Event))
    (Default|AddChallengeCompleted _currentsaveslot (Utilities|GetDisplayName _array_element))
    (if (Default|GetChallengeCompletedValue _currentsaveslot (Utilities|GetDisplayName _array_element))
      (Default|OnChallengeDone _array_element))))