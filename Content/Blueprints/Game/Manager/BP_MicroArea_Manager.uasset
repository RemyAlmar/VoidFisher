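; Manager for one data-table-defined micro area, tracking its creatures, parasites and unlock state through the save slot.
; On init it gathers BPI_MicroAreable actors in range, registers creature managers and parasites, and reports the area's fish total.
; First unlock spawns creatures and updates quests; catches are reported to the game instance.
; Parasite destruction is saved and quick-saved, so parasites saved as inactive are destroyed again on init.
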(event Custom|ED_OnCreatureCatched_Event
  (params (TargetCatched :type Actor%20Object%20Reference))
  (bind _data (Class|BPICatcheable|IGetCreatureData(Message) TargetCatched))
  (Default|HaveCatchFish (CallFunction|GetBPGameInstance) (Utilities|Struct|BreakS_MicroAreaInfo (CallFunction|GetDataMicroArea)) _data))

(event Custom|ED_OnAreaUnlocked_Event
  (params (Area :type E_MicroZone%20Enum :default "NewEnumerator4"))
  (if (Utilities|Enum|Equal(Enum) Area (Utilities|Struct|BreakS_MicroAreaInfo (CallFunction|GetDataMicroArea)))
    (if (not (Variables|Default|GetIsInitialized))
      (Variables|Default|SetIsInitialized true)
      (CallFunction|SetUnlock true)
      (CallFunction|InitCreaturesManager)
      (Default|UpdateNewQuest (CallFunction|GetBPGameInstance) (Utilities|Struct|BreakS_MicroAreaInfo (CallFunction|GetDataMicroArea)) (Variables|TypeCreature|GetCreatureTypeInArea))
      (Default|CallEDonAreaUnlocked Area))))

(event Custom|Parasite_ED_OnDestroyActor_Event
  (params (TargetToDestroy :type Actor%20Object%20Reference))
  (bind _microarea (Class|BPIMicroAreable|IGetMicroArea(Message) TargetToDestroy))
  (if (.IsActive (Default|GetParasiteActivity (Variables|/Game/Blueprints/Data/BP_GameInstance.BP_GameInstance_C|GetCurrentSaveSlot (CallFunction|GetBPGameInstance)) (Utilities|GetDisplayName TargetToDestroy) (Variables|Default|GetELevel) _microarea))
    (CallFunction|EDonCreatureCatchedEvent TargetToDestroy))
  (Default|SetParasiteActivity (Variables|/Game/Blueprints/Data/BP_GameInstance.BP_GameInstance_C|GetCurrentSaveSlot (CallFunction|GetBPGameInstance)) (Variables|Default|GetELevel) _microarea (Utilities|GetDisplayName TargetToDestroy) false)
  (Utilities|Array|RemoveItem (Variables|ActorInArea|GetParasitesInScene) TargetToDestroy)
  (Default|CallEDonParasiteDestroyed)
  (Default|QuickSaveSlot (CallFunction|GetBPGameInstance)))

(event EventIInitialize
  (EventDispatchers|AssignEDonAreaUnlocked (Variables|/Game/Blueprints/Data/BP_GameInstance.BP_GameInstance_C|GetCurrentSaveSlot (CallFunction|GetBPGameInstance)) (EventDispatchers|CreateEvent :!event Custom|ED_OnAreaUnlocked_Event))
  (CallFunction|GetActorsinRange)
  (CallFunction|Init)
  (Default|AddUnlockMicroArea (Variables|/Game/Blueprints/Data/BP_GameInstance.BP_GameInstance_C|GetCurrentSaveSlot (CallFunction|GetBPGameInstance)) (Utilities|Struct|BreakS_MicroAreaInfo (CallFunction|GetDataMicroArea)) (Variables|Params|GetIsUnlock))
  (bind _isunlock (Default|GetMicroAreaUnlock (Variables|/Game/Blueprints/Data/BP_GameInstance.BP_GameInstance_C|GetCurrentSaveSlot (CallFunction|GetBPGameInstance)) (Utilities|Struct|BreakS_MicroAreaInfo (CallFunction|GetDataMicroArea))))
  (CallFunction|SetUnlock _isunlock))

(fn ConstructionScript
  (|CallParentFunction))

(fn AddParasitestoSlotSave
  (params (CurrentActor :type BP%20Parasite%20Object%20Reference))
  ;[1 0.5379 0] Ajout du parasite dans la save, si il est inactif depuis la save alors destruction de celui ci
  (LocalVariables|SetCurrentActorName (Utilities|GetDisplayName CurrentActor))
  (bind _microarea (Class|BPIMicroAreable|IGetMicroArea(Message) CurrentActor))
  (LocalVariables|SetCurrentMicroArea _microarea)
  (if (.InData (Default|GetParasiteActivity (Variables|/Game/Blueprints/Data/BP_GameInstance.BP_GameInstance_C|GetCurrentSaveSlot (CallFunction|GetBPGameInstance)) (LocalVariables|GetCurrentActorName) (Variables|Default|GetELevel) (LocalVariables|GetCurrentMicroArea)))
    (LocalVariables|SetIsActive (.IsActive (Default|GetParasiteActivity (Variables|/Game/Blueprints/Data/BP_GameInstance.BP_GameInstance_C|GetCurrentSaveSlot (CallFunction|GetBPGameInstance)) (LocalVariables|GetCurrentActorName) (Variables|Default|GetELevel) (LocalVariables|GetCurrentMicroArea))))
    (else
      (LocalVariables|SetIsActive true)))
  (EventDispatchers|BindEventtoEDonDestroyActor CurrentActor (EventDispatchers|CreateEvent :!event Custom|Parasite_ED_OnDestroyActor_Event))
  (if (LocalVariables|GetIsActive)
    (Default|Initialize CurrentActor)
    (else
      (Utilities|Array|Add (Variables|ActorInArea|GetCurrentParasitesToDestroy) CurrentActor)))
  (Default|SetParasiteActivity (Variables|/Game/Blueprints/Data/BP_GameInstance.BP_GameInstance_C|GetCurrentSaveSlot (CallFunction|GetBPGameInstance)) (Variables|Default|GetELevel) (LocalVariables|GetCurrentMicroArea) (LocalVariables|GetCurrentActorName) (LocalVariables|GetIsActive)))

(fn GetActorsinRange
  (bind _output_get (Variables|ActorInArea|SetCreatureManagerWithInterfaceInRange (CallFunction|GetActorswithInterfaceinRange self "/Game/Blueprints/AddOn/Interface/BPI_MicroAreable.BPI_MicroAreable_C" (CallFunction|GetShapeRange))))
  (for _array_element _output_get
    (Class|BPIMicroAreable|ISetMicroArea(Message) _array_element (Utilities|Struct|BreakS_MicroAreaInfo (CallFunction|GetDataMicroArea)))
    (bind _asbp_parasite (Utilities|Casting|CastToBP_Parasite _array_element)
      (:then
        (Utilities|Array|AddUnique (Variables|ActorInArea|GetParasitesInScene) _asbp_parasite)
        (CallFunction|AddParasitestoSlotSave _asbp_parasite)
        (Utilities|Array|AddUnique (Variables|TypeCreature|GetCreatureTypeInArea) "NewEnumerator21"))
      (:CastFailed
        (bind _asbp_creature_manager (Utilities|Casting|CastToBP_CreatureManager _array_element))
        (Utilities|Array|AddUnique (Variables|ActorInArea|GetBP_CreatureManager) _asbp_creature_manager)
        (Default|AddManagertoSaveSlot _asbp_creature_manager)
        (EventDispatchers|BindEventtoEDonCreatureCatched _asbp_creature_manager (EventDispatchers|CreateEvent :!event Custom|ED_OnCreatureCatched_Event))
        (Utilities|Array|AddUnique (Variables|TypeCreature|GetCreatureTypeInArea) (.CreatureName (Utilities|Struct|BreakS_CreatureDetails (Variables|/Game/Blueprints/Game/Manager/BP_CreatureManager.BP_CreatureManager_C|GetCreatureWillSpawn _asbp_creature_manager))))
        (Utilities|Array|AddUnique (Variables|/Game/Blueprints/Data/BP_GameInstance.BP_GameInstance_C|GetCreatureAvailable (CallFunction|GetBPGameInstance)) (.CreatureName (Utilities|Struct|BreakS_CreatureDetails (Variables|/Game/Blueprints/Game/Manager/BP_CreatureManager.BP_CreatureManager_C|GetCreatureWillSpawn _asbp_creature_manager)))))))
  (for _array_element_2 (Variables|ActorInArea|GetCurrentParasitesToDestroy)
    (Default|EDDestroyActorEvent _array_element_2)))

(fn GetDataMicroArea
  (bind _dt_microarea (Variables|Params|GetDT_MicroArea))
  (bind _returnvalue (Utilities|GetDataTableRow (.datatable _dt_microarea) (.rowname _dt_microarea))
    (:then
      (return _returnvalue))))

(fn Init
  (bind _dt_microarea (Variables|Params|GetDT_MicroArea))
  (for _array_element (Variables|ActorInArea|GetBP_CreatureManager)
    (Variables|Default|SetTotal%20AI (+ (Variables|Default|GetTotal%20AI) (Variables|/Game/Blueprints/Game/Manager/BP_CreatureManager.BP_CreatureManager_C|GetNumberEntitiesToSpawn _array_element))))
  (bind _returnvalue (Utilities|GetDataTableRow (.datatable _dt_microarea) (.rowname _dt_microarea))
    (:then
      (Default|SetFishCountinMicroZone (CallFunction|GetBPGameInstance) (Utilities|Struct|BreakS_MicroAreaInfo _returnvalue) (Variables|Default|GetTotal%20AI)))))

(fn SetUnlock
  (params (IsUnlock :type Boolean))
  (LocalVariables|SetPreviousValue (Variables|Params|GetIsUnlock))
  (bind _output_get (Variables|Params|SetIsUnlock IsUnlock))
  (if _output_get
    (CallFunction|EDonAreaUnlockedEvent (Utilities|Struct|BreakS_MicroAreaInfo (CallFunction|GetDataMicroArea)))))

(fn InitCreaturesManager
  (for _array_element (Variables|ActorInArea|GetBP_CreatureManager)
    (Default|SpawnCreatures _array_element))
  (return))

(fn IGetPriority
  (return 1))