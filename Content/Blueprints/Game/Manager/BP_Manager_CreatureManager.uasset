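; Master manager that gathers every BP_CreatureManager in the level and culls them by player distance.
; On BeginPlay it loads each one's DataTable creature data and binds its creature-destroyed event.
; Tick starts or updates managers within their bounds plus a culling margin, and quits distant ones unless recently rendered.
; Creature destruction writes that manager's micro area, alive count and maximum to the current save slot.
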(event Custom|ED_ManagerCreature_OnCreatureDestroyed_Event
  (params (TargetCaller :type BP%20Creature%20Manager%20Object%20Reference))
  (Default|SetCreaturetoSpawnonManager (Variables|/Game/Blueprints/Data/BP_GameInstance.BP_GameInstance_C|GetCurrentSaveSlot (CallFunction|GetBPGameInstance)) (Utilities|GetDisplayName TargetCaller) (Utilities|Struct|MakeS_ManagerInfo (Variables|/Game/Blueprints/Game/Manager/BP_CreatureManager.BP_CreatureManager_C|GetCurrentMicroArea TargetCaller) (Default|GetCurrentCreaturesAlive TargetCaller) (Variables|/Game/Blueprints/Game/Manager/BP_CreatureManager.BP_CreatureManager_C|GetMaxNumberEntitiesToSpawn TargetCaller)))
  (Default|CallEDonChangeSaved (CallFunction|GetBPGameInstance)))

(event EventBeginPlay
  (CallFunction|SetAllManager)
  (CallFunction|InitManagers))

(event EventTick
  (params (DeltaSeconds :type Float%20%28single-precision%29))
  (for _array_element (Variables|Default|GetManagerList)
    (if (CallFunction|IsNeartoNotCull _array_element (Variables|/Game/Blueprints/Game/Manager/BP_CreatureManager.BP_CreatureManager_C|GetSizeBounds _array_element))
      (if (Variables|/Game/Blueprints/Game/Manager/BP_CreatureManager.BP_CreatureManager_C|GetIsActive _array_element) :!label _label
        (Default|IUpdate _array_element DeltaSeconds)
        (else
          (Default|IStart _array_element)))
      (elif (Variables|/Game/Blueprints/Game/Manager/BP_CreatureManager.BP_CreatureManager_C|GetIsActive _array_element)
        (if (Default|HasAnyActorRendered _array_element 1e+01)
          (goto _label)
          (else
            (Default|IQuit _array_element)))))))

(fn ConstructionScript)

(fn IsNeartoNotCull
  (params (Target :type Actor%20Object%20Reference) (Offset :type Float%20%28double-precision%29))
  (bind _bpgameinstance (CallFunction|GetBPGameInstance))
  (bind _returnvalue (Transformation|GetActorLocation Target))
  (bind _cullingmanager (Variables|Default|GetCullingManager))
  (bind _player (Default|GetPlayer _bpgameinstance))
  (bind _returnvalue_2 (+ Offset _cullingmanager))
  (bind _returnvalue_3 (Transformation|GetActorLocation _player))
  (bind _returnvalue_4 (Math|Vector|Distance(Vector) _returnvalue _returnvalue_3))
  (bind _returnvalue_5 (<= _returnvalue_4 _returnvalue_2))
  (Development|PrintText (Utilities|Text|FormatText "{x} has player in area = {y}" (Utilities|GetDisplayName Target) _returnvalue_5) true true "(R=1.000000,G=0.139179,B=0.000000,A=1.000000)" 0.0)
  (return _returnvalue_5))

(fn SetAllManager
  (bind _outactors (Actor|GetAllActorsOfClass "/Game/Blueprints/Game/Manager/BP_CreatureManager.BP_CreatureManager_C"))
  (Variables|Default|SetManagerList _outactors)
  (return))

(fn DisplayCullingDistance
  (for _array_element (Variables|Default|GetManagerList)
    (Collision|SphereTraceByChannel (Transformation|GetActorLocation _array_element) (Transformation|GetActorLocation _array_element) (+ (Variables|/Game/Blueprints/Game/Manager/BP_CreatureManager.BP_CreatureManager_C|GetSizeBounds _array_element) (Variables|Default|GetCullingManager)) "TraceTypeQuery1" false 0 "ForDuration" true "(R=0.931775,G=0.000000,B=1.000000,A=1.000000)" "(R=0.880913,G=0.000000,B=1.000000,A=1.000000)" 1e+01))
  (return))

(fn GetTotalCreaturesinLevel
  (for _array_element (Variables|Default|GetManagerList)
    (LocalVariables|SetpTotalCreatures (Default|GetTotalCreatures _array_element)))
  (return (LocalVariables|GetpTotalCreatures)))

(fn InitManagers
  (for _array_element (Variables|Default|GetManagerList)
    (Default|SetCreatureDatafromDataTable _array_element)
    (EventDispatchers|BindEventtoEDonCreatureDestroyed _array_element (EventDispatchers|CreateEvent :!event Custom|ED_ManagerCreature_OnCreatureDestroyed_Event)))
  (return))

(fn GetBPGameInstance
  (Variables|Default|GetBPGameInstance
    (:then
      _)
    (:else
      (bind _asbp_game_instance (Utilities|Casting|CastToBP_GameInstance (Game|GetGameInstance)))
      (Variables|Default|SetBPGameInstance _asbp_game_instance)))
  (return (Variables|Default|GetBPGameInstance)))