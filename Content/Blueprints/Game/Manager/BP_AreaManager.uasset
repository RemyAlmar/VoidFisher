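; BP_AreaManager is a manager that registers the level's micro-area managers and listens for their parasite-destroyed events.
; Its construction script finds every BP_MicroArea_Manager, maps each by its MicroArea value, assigns it this manager's Area and binds to its parasite-destroyed dispatcher.
; The parasite-destroyed handler only prints a French debug message, and BeginPlay just calls the parent.
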(event Custom|MicroArea_ED_OnParasiteDestroyed_Event
  (Development|PrintText "PARASITE DETRUIT" true true "(R=1.000000,G=0.000000,B=0.061744,A=1.000000)" 5.0))

(event EventBeginPlay
  (|CallParentFunction))

(fn ConstructionScript
  (|CallParentFunction)
  (bind _outactors (Actor|GetAllActorsOfClass "/Game/Blueprints/Game/Manager/BP_MicroArea_Manager.BP_MicroArea_Manager_C"))
  (for _array_element _outactors
    (Utilities|Map|Add (Variables|Default|GetMicroAreas) (Variables|/Game/Blueprints/Game/Manager/BP_MicroArea_Manager.BP_MicroArea_Manager_C|GetMicroArea _array_element) _array_element)
    (Variables|/Game/Blueprints/Game/Manager/BP_MicroArea_Manager.BP_MicroArea_Manager_C|SetELevel _array_element (Variables|Default|GetArea))
    (EventDispatchers|BindEventtoEDonParasiteDestroyed _array_element (EventDispatchers|CreateEvent :!event Custom|MicroArea_ED_OnParasiteDestroyed_Event))))