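; Manager that triggers the level's BP_QuestEvent actors when their bound quest is completed.
; On BeginPlay it binds to the game instance's quest-completed dispatcher and maps every quest event actor to its quest name.
; It also replays completion for quests in the current save slot, restoring their events.
; Matching events, found by a substring test on the quest name, run PreProcess then ActivateProcess.
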(event Custom|OnQuestCompleted_Event
  (params (QuestName :type Name))
  (CallFunction|PlayQuestsEventCorresponding QuestName))

(event EventBeginPlay
  (EventDispatchers|BindEventtoEDonQuestCompleted (CallFunction|GetBPGameInstance) (EventDispatchers|CreateEvent :!event Custom|OnQuestCompleted_Event))
  (CallFunction|GetAllQuestsEvent)
  (CallFunction|PlayAllQuestsEventCompleted))

(fn ConstructionScript)

(fn GetBPGameInstance
  (Variables|Default|GetBPGameInstance
    (:then
      _)
    (:else
      (bind _asbp_game_instance (Utilities|Casting|CastToBP_GameInstance (Game|GetGameInstance)))
      (Variables|Default|SetBPGameInstance _asbp_game_instance)))
  (return (Variables|Default|GetBPGameInstance)))

(fn GetAllQuestsEvent
  (bind _outactors (Actor|GetAllActorsOfClass "/Game/Blueprints/Game/Event/BP_QuestEvent.BP_QuestEvent_C"))
  (for _array_element _outactors
    (Utilities|Map|Add (Variables|Default|GetQuestEventList) _array_element (Utilities|Struct|MakeS_ArrayName (Default|GetQuestNameBinded _array_element))))
  (return))

(fn PlayAllQuestsEventCompleted
  (for _array_element (Default|GetQuestsCompleted (Variables|/Game/Blueprints/Data/BP_GameInstance.BP_GameInstance_C|GetCurrentSaveSlot (CallFunction|GetBPGameInstance)))
    (CallFunction|OnQuestCompletedEvent _array_element)))

(fn PlayQuestsEventCorresponding
  (params (TargetQuestName :type Name))
  (bind _keys (Utilities|Map|Keys (Variables|Default|GetQuestEventList)))
  (LocalVariables|SetQuestsEvents _keys)
  (bind _values (Utilities|Map|Values (Variables|Default|GetQuestEventList)))
  (for (_array_element _array_index) _values
    (if (Utilities|Array|ContainsItem (.name _array_element) TargetQuestName)
      (Default|PreProcess (Utilities|Array|Get(acopy) (LocalVariables|GetQuestsEvents) _array_index))
      (Default|ActivateProcess (Utilities|Array|Get(acopy) (LocalVariables|GetQuestsEvents) _array_index))))
  (return))