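; Event manager that opens doors in sequence as the player catches creatures.
; On BeginPlay it binds to the creature-destroyed dispatcher of every BP_CreatureManager and counts each destruction as a catch.
; Reaching the threshold starts the tutorial widget timer on BP_TutoColliderManager and signals the next door in the array to open.
; The counter and trigger flag reset only when that door is valid, so counting stops once no valid door remains.
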(event Custom|OnAllCreatureCatched
  (bind _doorindex (Variables|Default|GetDoorIndex))
  (bind _door (Variables|Parameter|GetDoor))
  (bind _output (Utilities|Array|Get(acopy) _door _doorindex))
  (Default|TutoWidget(Timer) (stale EventBeginPlay _returnvalue))
  (Utilities|IsValid _output
    (:Is%20Valid
      (Default|CallEDOpenDoor _output)
      (Math|Integer|IncrementInt _doorindex
        (:%20%20
          (Variables|Event|CreatureManager|SetCreatureNumberCatcher 0)
          (Variables|Default|SetEventTriggered false))))))

(event Custom|ED_CreatureManager_OnCreatureDestroyed
  (params (TargetCaller :type BP%20Creature%20Manager%20Object%20Reference))
  (if (not (Variables|Default|GetEventTriggered))
    (bind _result (Math|Integer|IncrementInt (Variables|Event|CreatureManager|GetCreatureNumberCatcher))
      (:%20%20
        (if (>= _result (Variables|Event|CreatureManager|GetCreatureNumberCatchedBeforeEvent))
          (Variables|Default|SetEventTriggered (>= _result (Variables|Event|CreatureManager|GetCreatureNumberCatchedBeforeEvent)))
          (CallFunction|OnAllCreatureCatched))))))

(event EventBeginPlay
  (bind _returnvalue (Actor|GetActorOfClass "/Game/Blueprints/Onboarding/BP_TutoColliderManager.BP_TutoColliderManager_C"))
  (bind _outactors (Actor|GetAllActorsOfClass "/Game/Blueprints/Game/Manager/BP_CreatureManager.BP_CreatureManager_C"))
  (bind _output_get (Variables|Event|CreatureManager|SetCreatureManager _outactors))
  (for _array_element _output_get
    (EventDispatchers|BindEventtoEDonCreatureDestroyed _array_element (EventDispatchers|CreateEvent :!event Custom|ED_CreatureManager_OnCreatureDestroyed)))
  (bind _asbp_game_instance (Utilities|Casting|CastToBP_GameInstance (Game|GetGameInstance)))
  (Variables|Default|SetGameInstance _asbp_game_instance)
  (Variables|Default|SetEventTriggered false))

(fn ConstructionScript)