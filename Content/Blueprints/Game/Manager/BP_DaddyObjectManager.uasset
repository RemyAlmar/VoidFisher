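; Level manager that tracks collectible BP_DaddyObject actors through the current save slot.
; On BeginPlay it gathers every such actor, registers its display name and data object in the save, and caches its collected state.
; Already collected objects are destroyed; the rest get a bound collection event that marks them collected in the save slot.
; Save entries are keyed by actor display name.
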(event Custom|ED_OnObjectCollected_Event
  (params (Target :type BP%20Daddy%20Object%20Object%20Reference))
  (Default|ChangeDaddyObjectValue (Variables|/Game/Blueprints/Data/BP_GameInstance.BP_GameInstance_C|GetCurrentSaveSlot (Variables|Default|GetBPGame%20Instance)) (Utilities|GetDisplayName Target) true))

(event EventBeginPlay
  (bind _asbp_game_instance (Utilities|Casting|CastToBP_GameInstance (Game|GetGameInstance)))
  (Variables|Default|SetBPGame%20Instance _asbp_game_instance)
  (bind _outactors (Actor|GetAllActorsOfClass "/Game/Blueprints/Game/Miscellanious/BP_DaddyObject.BP_DaddyObject_C"))
  (CallFunction|InitObjects _outactors))

(fn ConstructionScript)

(fn InitObjects
  (params (Array :type Array%20of%20BP%20Daddy%20Object%20Object%20References))
  (bind _bpgame_instance (Variables|Default|GetBPGame%20Instance))
  (bind _currentsaveslot (Variables|/Game/Blueprints/Data/BP_GameInstance.BP_GameInstance_C|GetCurrentSaveSlot _bpgame_instance))
  (for _array_element Array
    (LocalVariables|SetCurrentObject _array_element)
    (Default|AddDaddyObjectValue _currentsaveslot (Utilities|GetDisplayName (LocalVariables|GetCurrentObject)))
    (Default|AddDaddyObjectData _currentsaveslot "" (Variables|/Game/Blueprints/Game/Miscellanious/BP_DaddyObject.BP_DaddyObject_C|GetDataObject (LocalVariables|GetCurrentObject)))
    (Utilities|Map|Add (Variables|Default|GetDaddyObjectsCollected) (LocalVariables|GetCurrentObject) (Default|GetDaddyObjectValue (Variables|/Game/Blueprints/Data/BP_GameInstance.BP_GameInstance_C|GetCurrentSaveSlot (Variables|Default|GetBPGame%20Instance)) (Utilities|GetDisplayName (LocalVariables|GetCurrentObject))))
    (if (Default|GetDaddyObjectValue (Variables|/Game/Blueprints/Data/BP_GameInstance.BP_GameInstance_C|GetCurrentSaveSlot (Variables|Default|GetBPGame%20Instance)) (Utilities|GetDisplayName (LocalVariables|GetCurrentObject)))
      (Actor|DestroyActor (LocalVariables|GetCurrentObject))
      (else
        (EventDispatchers|BindEventtoEDonCollected (LocalVariables|GetCurrentObject) (EventDispatchers|CreateEvent :!event Custom|ED_OnObjectCollected_Event))))))