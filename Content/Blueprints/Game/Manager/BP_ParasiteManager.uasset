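; Level manager for BP_Parasite actors that keeps each one's active state in the current save slot.
; On BeginPlay it registers every parasite, destroys those saved as inactive, and saves later destructions as inactive through a bound event.
; It also holds unfinished area-spawning tools: mesh vertices gathered within a radius and weighted per actor, but the spawn code is disconnected.
; Tick prints remaining parasite names as debug output.
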(event Custom|Parasite_ED_OnDestroyActor_Event
  (params (TargetToDestroy :type Actor%20Object%20Reference))
  (Default|SetParasiteActivity (Variables|/Game/Blueprints/Data/BP_GameInstance.BP_GameInstance_C|GetCurrentSaveSlot (Variables|Default|GetBP%20Game%20Instance)) (Variables|Param|GetELevel) (Utilities|GetDisplayName TargetToDestroy) false)
  (Utilities|Array|RemoveItem (Variables|HandleActors|GetParasiteInScene) TargetToDestroy))

(event EventBeginPlay
  (bind _asbp_game_instance (Utilities|Casting|CastToBP_GameInstance (Game|GetGameInstance)))
  (Variables|Default|SetBP%20Game%20Instance _asbp_game_instance)
  (bind _outactors (Actor|GetAllActorsOfClass "/Game/Blueprints/AI/Pawn/BP_Parasite.BP_Parasite_C"))
  (bind _output_get (Variables|HandleActors|SetParasiteInScene _outactors))
  (Variables|Default|SetTotalActors (Utilities|Array|Length _output_get))
  (for _array_element (Variables|HandleActors|GetParasiteInScene)
    (CallFunction|AddParasitestoSlotSave _array_element))
  (for _array_element_2 (Variables|HandleActors|GetCurrentActorsToDestroy)
    (Default|CallEDDestroyActor _array_element_2)))

(event EventTick
  (params (DeltaSeconds :type Float%20%28single-precision%29))
  (bind _parasiteinscene (Variables|HandleActors|GetParasiteInScene))
  (if (Utilities|Array|IsNotEmpty _parasiteinscene)
    (for _array_element _parasiteinscene
      (Development|PrintText (Utilities|Text|FormatText "Parasite Name In Scene : {x}" (Utilities|GetDisplayName _array_element)) true true "(R=0.160779,G=1.000000,B=0.000000,A=1.000000)" 0.0))))

(fn ConstructionScript
  (Components|Sphere|SetSphereRadius (Variables|Default|GetSphere) (Variables|Param|Bound|Size|GetSize) true)
  (Components|Box|SetBoxExtent (Variables|Default|GetBox) (Math|Conversions|ToVector(Float) (Variables|Param|Bound|Size|GetSize)) true)
  (FUNC|SetShape))

(fn SetShape
  (switch Utilities|FlowControl|Switch|SwitchonE_CollisionShape (Variables|Param|Bound|Shape|GetShape)
    (:NewEnumerator1
      (Variables|Default|SetShape%20Collision (Variables|Default|GetSphere)))
    (:NewEnumerator2
      (Variables|Default|SetShape%20Collision (Variables|Default|GetBox))))
  (Rendering|SetVisibility (Variables|Default|GetShape%20Collision) true false)
  (Development|SetHiddeninGame (Variables|Default|GetShape%20Collision) (Variables|Param|Bound|Shape|GetHiddenInGame) false)
  (return))

(fn SpawnObjects
  (bind _keys (Utilities|Map|Keys (Variables|Param|ActorsInArea|GetActorsInArea)))
  (for _array_element _keys ; Parcours les acteurs
    (bind _output_get (LocalVariables|SetActor _array_element))
    (bind _output_get_2 (LocalVariables|SetS_LocalActorData (.Value (Utilities|Map|Find (Variables|Param|ActorsInArea|GetActorsInArea) _output_get))))
    (for (_ _array_index) (.vector (Utilities|Struct|BreakS_MeshDataPonderation _output_get_2)) ; Set un array des Vertex prochainement Utilisé
      (Utilities|Map|Add (LocalVariables|GetVertexCanUsed) _array_index false))
    (for _index (range 1 (FUNC|HandleValues|GetPonderationValue (LocalVariables|GetActor))) ; Va loop pour Spawn tous les objets prévu selon sa pondération
      (bind _keys_2 (Utilities|Map|Keys (LocalVariables|GetVertexCanUsed)))
      (for _array_element_2 _keys_2
        (for _array_element_3 (.vector (.vertices (LocalVariables|GetS_LocalActorData)))
          (LocalVariables|SetIndexToSpawn (Math|Random|RandomIntegerinRange 0 (Utilities|Array|LastIndex (.vector (.vertices (LocalVariables|GetS_LocalActorData)))))))))))

(fn RemoveObjectSpawned
  (for _array_element (Variables|ObjectSpawned|GetParasites)
    (Actor|DestroyActor _array_element))
  (Utilities|Array|Clear (Variables|ObjectSpawned|GetParasites)))

(fn GetActorsinShape
  (for _array_element (Variables|Param|ClassWhereSpawn|GetActor%20ClassToSpawnParasites)
    (bind _outactors (Actor|GetAllActorsOfClass _array_element))
    (for _array_element_2 _outactors
      (bind _output_get (LocalVariables|SetActor _array_element_2))
      (if (<= (Math|Vector|Distance(Vector) (Transformation|GetActorLocation _output_get) (Transformation|GetActorLocation)) (Variables|Param|Bound|Size|GetSize))
        (Utilities|IsValid (Actor|GetComponentbyClass (LocalVariables|GetActor) "/Script/Engine.StaticMeshComponent")
          (:Is%20Valid
            (bind (_vertices _triangles _normals) (Class|KismetProceduralMeshLibrary|GetSectionfromStaticMesh (Variables|/Script/Engine.StaticMeshComponent|GetStaticMesh (Actor|GetComponentbyClass (LocalVariables|GetActor) "/Script/Engine.StaticMeshComponent"))))
            (Utilities|Map|Add (Variables|Param|ActorsInArea|GetActorsInArea) (LocalVariables|GetActor) (Utilities|Struct|MakeS_MeshDataPonderation 1 (Utilities|Struct|MakeS_ArrayVector _vertices) (Utilities|Struct|MakeS_ArrayVector _normals))))))))
  (return))

(fn SetSumPonderation
  (Variables|Default|SetSumPonderation 0)
  (bind _keys (Utilities|Map|Keys (Variables|Param|ActorsInArea|GetActorsInArea)))
  (for _array_element _keys
    (Variables|Default|SetSumPonderation (+ (Variables|Default|GetSumPonderation) (.ponderation (.Value (Utilities|Map|Find (Variables|Param|ActorsInArea|GetActorsInArea) _array_element))))))
  (return (Variables|Default|GetSumPonderation)))

(fn DisplayPond
  (Variables|Default|SetSumPonderation (FUNC|HandleValues|SetSumPonderation))
  (bind _keys (Utilities|Map|Keys (Variables|Param|ActorsInArea|GetActorsInArea)))
  (for _array_element _keys
    (Development|PrintText (Utilities|Text|FormatText "{y} has {x} Ponderation and can spawn {z} parasites" (Utilities|GetDisplayName _array_element) (.ponderation (.Value (Utilities|Map|Find (Variables|Param|ActorsInArea|GetActorsInArea) _array_element))) (FUNC|HandleValues|GetPonderationValue _array_element)) true true "(R=0.206200,G=1.000000,B=0.000000,A=1.000000)" 5e+01))
  (return))

(fn ClearActorsinShape
  (FUNC|RemoveObjectSpawned)
  (Utilities|Map|Clear (Variables|Param|ActorsInArea|GetActorsInArea)))

(fn GetPonderationValue
  (params (Key :type Actor%20Object%20Reference%20%28by%20ref%29))
  (return (Math|Float|Round (/ (* (.ponderation (.Value (Utilities|Map|Find (Variables|Param|ActorsInArea|GetActorsInArea) Key))) (Variables|Param|Spawn|GetParasitesNumberToSpawn)) (Variables|Default|GetSumPonderation)))))

(fn GetVertexLocation
  (params (Vertex :type Vector) (Target :type Actor%20Object%20Reference))
  (return (+ (Transformation|GetActorLocation Target) Vertex)))

(fn AddParasitestoSlotSave
  (params (TargetActor :type Actor%20Object%20Reference%20%28by%20ref%29))
  ;[1 0.5379 0] Ajout du parasite dans la save, si il est inactif depuis la save alors destruction de celui ci
  (bind _asbp_parasite (Utilities|Casting|CastToBP_Parasite TargetActor))
  (bind _output_get (LocalVariables|SetCurrentActor _asbp_parasite))
  (LocalVariables|SetCurrentActorName (Utilities|GetDisplayName _output_get))
  (if (.InData (Default|ActorIsActive (Variables|/Game/Blueprints/Data/BP_GameInstance.BP_GameInstance_C|GetCurrentSaveSlot (Variables|Default|GetBP%20Game%20Instance)) (LocalVariables|GetCurrentActorName) (Variables|Param|GetELevel)))
    (LocalVariables|SetIsActive (.IsActive (Default|ActorIsActive (Variables|/Game/Blueprints/Data/BP_GameInstance.BP_GameInstance_C|GetCurrentSaveSlot (Variables|Default|GetBP%20Game%20Instance)) (LocalVariables|GetCurrentActorName) (Variables|Param|GetELevel))))
    (else
      (LocalVariables|SetIsActive true)))
  (EventDispatchers|BindEventtoEDonDestroyActor (LocalVariables|GetCurrentActor) (EventDispatchers|CreateEvent :!event Custom|Parasite_ED_OnDestroyActor_Event))
  (if (LocalVariables|GetIsActive)
    _
    (else
      (Utilities|Array|Add (Variables|HandleActors|GetCurrentActorsToDestroy) (LocalVariables|GetCurrentActor))))
  (Default|SetParasiteActivity (Variables|/Game/Blueprints/Data/BP_GameInstance.BP_GameInstance_C|GetCurrentSaveSlot (Variables|Default|GetBP%20Game%20Instance)) (Variables|Param|GetELevel) (LocalVariables|GetCurrentActorName) (LocalVariables|GetIsActive)))