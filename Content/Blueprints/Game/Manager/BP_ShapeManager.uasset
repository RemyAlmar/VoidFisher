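; BP_ShapeManager defines a configurable sphere or box volume that supplies its range and random points inside it.
; The construction script sizes the selected component from a per-shape size map and sets its visibility, while the Capsule option is unimplemented.
; Random points are centred on the actor location, with sphere points using a minimum radius percentage.
; BeginPlay caches the BP_GameInstance reference.
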(event EventBeginPlay
  (bind _asbp_game_instance (Utilities|Casting|CastToBP_GameInstance (Game|GetGameInstance)))
  (Variables|Default|SetBPGame%20Instance _asbp_game_instance))

(fn ConstructionScript
  (CallFunction|SetShape))

(fn SetShape
  (bind _box (Variables|Default|GetBox))
  (bind _shapesize (Variables|Shape|GetShapeSize))
  (bind _shape (Variables|Shape|GetShape))
  (bind _sphere (Variables|Default|GetSphere))
  (bind _output_get (LocalVariables|SetSize (.Value (Utilities|Map|Find _shapesize _shape))))
  (Utilities|Map|Add _shapesize _shape _output_get)
  (switch Utilities|FlowControl|Switch|SwitchonE_CollisionShape (Variables|Shape|GetShape)
    (:NewEnumerator1
      (Components|Sphere|SetSphereRadius _sphere (LocalVariables|GetSize) true)
      (Variables|Default|SetShapeComponent _sphere))
    (:NewEnumerator0
      _)
    (:NewEnumerator2
      (Components|Box|SetBoxExtent _box (Math|Conversions|ToVector(Float) (LocalVariables|GetSize)) true)
      (Variables|Default|SetShapeComponent _box)))
  (Rendering|SetVisibility (Variables|Default|GetShapeComponent) true false)
  (Development|SetHiddeninGame (Variables|Default|GetShapeComponent) (Variables|Shape|GetHiddenInGame) false))

(fn GetShapeRange
  (return (.Value (Utilities|Map|Find (Variables|Shape|GetShapeSize) (Variables|Shape|GetShape)))))

(fn GetRandomPointinShape
  (switch Utilities|FlowControl|Switch|SwitchonE_CollisionShape (Variables|Shape|GetShape)
    (:NewEnumerator1
      (LocalVariables|SetPointLocation (CallFunction|GetRandomPointinSphere (Transformation|GetActorLocation) 0.2 (Variables|/Script/Engine.SphereComponent|GetSphereRadius (Variables|Default|GetSphere)) 0.0)))
    (:NewEnumerator2
      (LocalVariables|SetPointLocation (Math|Random|RandomPointinBoundingBox (Transformation|GetActorLocation) (Variables|/Script/Engine.BoxComponent|GetBoxExtent (Variables|Default|GetBox))))))
  (return (LocalVariables|GetPointLocation)))