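; Quest-gated event actor for a wall that shatters when a dashing actor hits it.
; A hit on GeoMesh checks the bound quest, the approximate direction and the BPC_Dash state, printing debug text for some failures.
; Success destroys GeoMesh, reveals the hidden GeoChaos and triggers the FSMasterField to break it.
; Global time dilation, applied every Tick, drops into slow motion on destruction and is restored after a short delay.
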(event Custom|OnGeoOverlap_Event
  (params (OverlappedActor :type Actor%20Object%20Reference) (OtherActor :type Actor%20Object%20Reference)))

(event Custom|OnGeoHit_Event
  (params (SelfActor :type Actor%20Object%20Reference) (OtherActor :type Actor%20Object%20Reference) (NormalImpulse :type Vector) (Hit :type Hit%20Result%20Structure%20%28by%20ref%29))
  (bind _returnvalue (Actor|GetComponentbyClass OtherActor "/Game/Blueprints/AddOn/Components/BPC_Dash.BPC_Dash_C"))
  (if (Default|GetQuestValue (Variables|/Game/Blueprints/Data/BP_GameInstance.BP_GameInstance_C|GetCurrentSaveSlot (CallFunction|GetBPGameInstance)) (CallFunction|GetQuestNameBinded))
    (if (CallFunction|IsinDirectionApproximately OtherActor self 0.7)
      (Utilities|IsValid _returnvalue
        (:Is%20Valid
          (if (Variables|/Game/Blueprints/AddOn/Components/BPC_Dash.BPC_Dash_C|GetIsInDash _returnvalue)
            (CallFunction|Process)
            (Utilities|FlowControl|Delay 2.0)
            (CallFunction|SetTargetTimeDilatation 1.0)
            (else
              (Development|PrintText "Is not in Dash" true true "(R=1.000000,G=0.000000,B=0.201022,A=1.000000)" 3.0))))))
    (else
      (Development|PrintText "Quest No Completed" true true "(R=1.000000,G=0.000000,B=0.275073,A=1.000000)" 1e+01))))

(event EventBeginPlay
  (Rendering|SetActorHiddenInGame (Variables|Default|GetGeoChaos) true)
  (CallFunction|Bind))

(event EventTick
  (params (DeltaSeconds :type Float%20%28single-precision%29))
  (|CallParentFunction DeltaSeconds)
  (Utilities|Time|SetGlobalTimeDilation (Variables|Default|GetCurrentTimeDilatation)))

(fn ConstructionScript
  (|CallParentFunction))

(fn Bind
  (bind _geomesh (Variables|Default|GetGeoMesh)
    (:then
      (Collision|BindEventtoOnActorHit _geomesh (EventDispatchers|CreateEvent :!event Custom|OnGeoHit_Event))
      (return))
    (:else)))

(fn Process
  (CallFunction|SetTargetTimeDilatation 0.2)
  (Rendering|SetActorHiddenInGame (Variables|Default|GetGeoChaos) false)
  (EventDispatchers|UnbindallEventsfromOnActorBeginOverlap (Variables|Default|GetGeoMesh))
  (Actor|DestroyActor (Variables|Default|GetGeoMesh))
  (Default|CETrigger (Variables|Default|GetFSMasterField))
  (Development|PrintText "DESTRUCTION" true true "(R=1.000000,G=0.721644,B=0.000000,A=1.000000)" 5.0)
  (|CallParentFunction))

(fn PreProcess
  (|CallParentFunction))