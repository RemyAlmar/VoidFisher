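; BP_QuestEvent is an actor for quest events, exposing its QuestID row name and empty Process and PreProcess functions, apparently for child overrides.
; ActivateProcess runs Process when AutoProcess is set.
; It also drives slow motion: setters store a target and toggle Tick, which eases global time dilation at a constant rate.
; Tick switches itself off once dilation rises back to normal speed.
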(event Custom|ActivateProcess
  (if (Variables|QuestData|GetAutoProcess)
    (CallFunction|Process)))

(event EventTick
  (params (DeltaSeconds :type Float%20%28single-precision%29))
  (CallFunction|SetTimeDilatation (Variables|Default|GetTargetTimeDilatation)))

(fn ConstructionScript)

(fn Process)

(fn GetQuestNameBinded
  (return (.rowname (Variables|QuestData|GetQuestID))))

(fn ActiveSlowMotion
  (params (tickEnabled :type Boolean) (TargetTimeDilatation :type Float%20%28double-precision%29))
  (Actor|Tick|SetActorTickEnabled tickEnabled)
  (Variables|Default|SetTargetTimeDilatation TargetTimeDilatation))

(fn SetTimeDilatation
  (params (Target :type Float%20%28double-precision%29))
  (LocalVariables|SetPreviousValue (Variables|Default|GetCurrentTimeDilatation))
  (bind _output_get (Variables|Default|SetCurrentTimeDilatation (Math|Interpolation|FInterptoConstant (Variables|Default|GetCurrentTimeDilatation) Target (Utilities|Time|GetWorldDeltaSeconds) (Variables|Default|GetInterpSpeedDilatation))))
  (Utilities|Time|SetGlobalTimeDilation _output_get)
  (if (!= (Variables|Default|GetCurrentTimeDilatation) (LocalVariables|GetPreviousValue))
    (if (> (Variables|Default|GetCurrentTimeDilatation) (LocalVariables|GetPreviousValue))
      (if (>= (Variables|Default|GetCurrentTimeDilatation) 1.0)
        (Utilities|Time|SetGlobalTimeDilation 1.0)
        (Actor|Tick|SetActorTickEnabled false)))))

(fn SetTargetTimeDilatation
  (params (TargetTimeDilatation :type Float%20%28double-precision%29))
  (Variables|Default|SetTargetTimeDilatation TargetTimeDilatation)
  (Actor|Tick|SetActorTickEnabled true))

(fn PreProcess)