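; Quest event actor that shows constellation actors for completed quests and hides those for unfinished ones.
; The construction script finds every BP_Constellations actor, matches its creature type name to a DT_Quest row, then records the quest ID and groups the actor under that quest.
; Process sets each group's visibility through an interface message, based on the current save slot's completed quests, then calls the parent.
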(fn ConstructionScript
  (|CallParentFunction)
  (CallFunction|ClearQuestID)
  (Utilities|Map|Clear (Variables|Default|GetActorsToShow))
  (CallFunction|SetAllActors))

(fn PreProcess
  (|CallParentFunction))

(fn Process
  (CallFunction|ShowActorsOfQuests)
  (|CallParentFunction))

(fn SetActorstoShowVisible
  (params (QuestName :type Name%20%28by%20ref%29) (IsVisible :type Boolean))
  (for _array_element (.actors (.Value (Utilities|Map|Find (Variables|Default|GetActorsToShow) QuestName)))
    (Class|BPIRendereable|ISetVisibility(Message) _array_element IsVisible))
  (return))

(fn ShowActorsOfQuests
  (bind _keys (Utilities|Map|Keys (Variables|Default|GetActorsToShow)))
  (for _array_element _keys
    (LocalVariables|SetIsVisible (Utilities|Array|ContainsItem (Default|GetQuestsCompleted (Variables|/Game/Blueprints/Data/BP_GameInstance.BP_GameInstance_C|GetCurrentSaveSlot (CallFunction|GetBPGameInstance))) _array_element))
    (CallFunction|SetActorstoShowVisible _array_element (LocalVariables|GetIsVisible))))

(fn AddActortoShow
  (params (Key :type Name%20%28by%20ref%29) (NewItem :type Actor%20Object%20Reference%20%28by%20ref%29))
  (bind _actorstoshow (Variables|Default|GetActorsToShow))
  (LocalVariables|SetCurrentArrayActor (.Value (Utilities|Map|Find _actorstoshow Key)))
  (Utilities|Array|Add (.actors (LocalVariables|GetCurrentArrayActor)) NewItem)
  (Utilities|Map|Add _actorstoshow Key (LocalVariables|GetCurrentArrayActor)))

(fn SetAllActors
  (bind _outactors (Actor|GetAllActorsOfClass "/Game/Blueprints/Game/Environment/BP_Constellations.BP_Constellations_C"))
  (for _array_element _outactors
    (bind _creaturetypename (Default|IGetCreatureTypeName _array_element))
    (if (!= (CallFunction|GetRowNamefromString "/Game/Blueprints/Data/DataTable/DT_Quest.DT_Quest" 2 _creaturetypename) "")
      (LocalVariables|SetCurrentName (CallFunction|GetRowNamefromString "/Game/Blueprints/Data/DataTable/DT_Quest.DT_Quest" 2 _creaturetypename))
      (Utilities|Array|Add (Variables|Default|GetQuestID) (Utilities|Struct|MakeDataTableRowHandle "/Game/Blueprints/Data/DataTable/DT_Quest.DT_Quest" (LocalVariables|GetCurrentName)))
      (CallFunction|AddActortoShow (LocalVariables|GetCurrentName) _array_element))))