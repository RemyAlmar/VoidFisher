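; BP_EndQuestEvent is a quest event that handles the game's ending once all quests are completed.
; Its Process notifies the game instance that all big creatures are caught when every quest is done, then runs the parent logic.
; The game instance's EndGame dispatcher triggers EndCinematic, which unpauses and starts a ship HUD fade-in.
; When that fade ends, it rechecks quest completion, shows the outro cinematic widget and fades out.
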(event Custom|GameInstance_ED_EndGame_event
  (CallFunction|EndCinematic))

(event Custom|ED_EndFadeIn_Event
  (if (CallFunction|HasAllQuestCompleted)
    (bind _returnvalue (UserInterface|CreateWidget "/Game/Cinematic/UI_CinematicOutro.UI_CinematicOutro_C"))
    (UserInterface|Viewport|AddtoViewport _returnvalue 9999)
    (Default|FadeOut (Default|GetHUDShip (Default|GetPlayer (CallFunction|GetBPGameInstance))))))

(event Custom|ED_EndFadeOut_Event)

(event EventBeginPlay
  (|CallParentFunction)
  (EventDispatchers|BindEventtoEDEndGame (CallFunction|GetBPGameInstance) (EventDispatchers|CreateEvent :!event Custom|GameInstance_ED_EndGame_event)))

(fn ConstructionScript
  (|CallParentFunction))

(fn EndCinematic
  (bind _bpgame_instance (CallFunction|GetBPGameInstance))
  (bind _player (Default|GetPlayer _bpgame_instance))
  (bind _hud_ship (Default|GetHUDShip _player))
  (Game|SetGamePaused false)
  (EventDispatchers|BindEventtoEDonFadeinEnd _hud_ship (EventDispatchers|CreateEvent :!event Custom|ED_EndFadeIn_Event))
  (EventDispatchers|BindEventtoEDonFadeOutEnd _hud_ship (EventDispatchers|CreateEvent :!event Custom|ED_EndFadeOut_Event))
  (Default|Fadein (Default|GetHUDShip (Default|GetPlayer (CallFunction|GetBPGameInstance)))))

(fn Process
  (if (CallFunction|HasAllQuestCompleted)
    (Default|AllBigCreatureCatchedEvent (CallFunction|GetBPGameInstance)))
  (|CallParentFunction))