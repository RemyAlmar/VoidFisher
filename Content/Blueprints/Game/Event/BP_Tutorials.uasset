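; Tutorial manager that guides the player through first-time onboarding, plus plunger-tool and wall pop-up tips.
; On BeginPlay it binds to game instance, player, spaceport, Purple Moon and tutorial collider events, creating UI_PopUpTuTo if the save enables tutorials.
; BranchFirstTuto gates first-tutorial steps through an ordered completion map.
; Events advance the widget with timed delays and retarget radar pings toward flows, Purple Moon, parasites, creatures and the spaceport.
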(event Custom|ED_PlayerInTutorialZone
  (params (Tag :type Name))
  ;[0.571 1 0.7923] Collider
  (switch name Tag
    (:Wall
      (bind _current_widget (Variables|Private|Widget|GetCurrent%20Widget)
        (:then
          (Default|WallTutoVisibility _current_widget true)
          (Utilities|FlowControl|Delay 1e+01)
          (Default|WallTutoVisibility _current_widget false))
        (:else
          (bind _returnvalue (UserInterface|CreateWidget "/Game/Blueprints/Widgets/Tuto/UI_PopUpTuTo.UI_PopUpTuTo_C" 0 false false 0 0 0 "/Game/SFX/Sounds/NEW_OGG/Menu_UI_UX/Menu/SFX_ButtonHoveredMenu_Cue.SFX_ButtonHoveredMenu_Cue"))
          (UserInterface|Viewport|AddtoViewport _returnvalue 0)
          (Default|WallTutoVisibility _returnvalue true)
          (Utilities|FlowControl|Delay 1e+01)
          (Widget|RemovefromParent _returnvalue))))))

(event Custom|ED_PlayerInSpaceport)

(event Custom|ED_OnParasiteDestroyed
  (bind _current_widget (Variables|Private|Widget|GetCurrent%20Widget))
  ;[0.9723 1 0.2825] Tool unlocked
  (bind _current_widget_2 (Variables|Private|Widget|GetCurrent%20Widget)
    (:then
      (Default|PlungerTutorial _current_widget_2)
      (Default|ClearAllPings (Variables|Default|GetBPC_Radar))
      (Utilities|FlowControl|Delay 1e+01)
      (Default|PlungerTutorial (Variables|Private|Widget|GetCurrent%20Widget))
      (Utilities|FlowControl|Delay 1e+01)
      (Default|PlungerTutorial _current_widget)
      (Default|PlungerTutoVisibility _current_widget false))
    (:else)))

(event Custom|ED_PlayerExitMicroArea
  (params (MicroArea :type E_MicroZone%20Enum :default "NewEnumerator4"))
  ;[0.5431 1 0.6432] Player in micro zone
  (bind _current_widget (Variables|Private|Widget|GetCurrent%20Widget)
    (:then
      (Default|PlayerNotinZone _current_widget))
    (:else)))

(event Custom|ED_SpaceportClose
  (bind _current_widget (Variables|Private|Widget|GetCurrent%20Widget)
    (:then
      (Default|HideTutorial _current_widget true)
      (Default|ShowAllPings (Variables|Default|GetBPC_Radar)))
    (:else)))

(event Custom|ED_CinematicSpaceportStarted
  ;[0.4394 0.5514 1] EndFirstTutorial
  (bind _current_widget (Variables|Private|Widget|GetCurrent%20Widget)
    (:then
      (Default|HideTutorial _current_widget false)
      (Utilities|BranchFirstTuto 5
        (:True
          (Default|FirstTutorial (Variables|Private|Widget|GetCurrent%20Widget))
          (Default|ClearAllPings (Variables|Default|GetBPC_Radar))
          (Variables|Default|SetFirstTutorialActive false))
        (:False
          (Default|HideAllPings (Variables|Default|GetBPC_Radar) :!label _label)
          (if (not (Variables|Default|GetQuestCompleted))
            (Default|SetCurrentTarget (Variables|Default|GetBPC_Radar) (Private|GetValues|GetSpaceport))
            (Variables|Default|SetQuestCompleted true)))))
    (:else
      (goto _label))))

(event Custom|PlayerHaveMoveAndTurn
  ;[1 1 1] 1
  (if (Variables|Default|GetFirstTutorialActive)
    (Utilities|Timer 5.0
      (:Completed
        (Utilities|BranchFirstTuto 1
          (:True
            (Utilities|Map|Add (Variables|Private|Widget|Getb_FirstTuto) 1 true)
            (bind _current_widget (Variables|Private|Widget|GetCurrent%20Widget)
              (:then
                (Default|FirstTutorial _current_widget)
                (Default|SetCurrentTarget (Variables|Default|GetBPC_Radar) (CallFunction|GetPingNear true "Flow")))
              (:else))))))))

(event Custom|ED_QuestCompleted
  (params (QuestName :type Name))
  (bind _bpc_radar (Variables|Default|GetBPC_Radar))
  ;[0.8926 0.7054 1] Quest Completed
  (if (Variables|Default|GetFirstTutorialActive)
    (Utilities|BranchFirstTuto 4
      (:True
        (if (== QuestName (Utilities|Array|Get(acopy) (Default|GetQuestbyCreatureType (Private|GetValues|GetBPGameInstance) "NewEnumerator16")))
          (Utilities|Map|Add (Variables|Private|Widget|Getb_FirstTuto) 4 true)
          (bind _current_widget (Variables|Private|Widget|GetCurrent%20Widget)
            (:then
              (Default|FirstTutorial _current_widget)
              (Default|ClearAllPings _bpc_radar)
              (Utilities|FlowControl|Delay 0.2) ; évite que le ping du spaceport se fasse clear
              (Default|SetCurrentTarget _bpc_radar (Private|GetValues|GetSpaceport))
              (Utilities|FlowControl|Delay 2.0)
              (bind _current_widget_2 (Variables|Private|Widget|GetCurrent%20Widget)
                (:then
                  (Default|PauseTutorial _current_widget_2))
                (:else)))
            (:else)))))
    (elif (Variables|Default|GetQuestCompleted)
      (Variables|Default|SetQuestCompleted false)
      (Default|SetCurrentTarget (Variables|Default|GetBPC_Radar) (Private|GetValues|GetSpaceport)))))

(event Custom|ED_ToolUnlock
  (params (ToolShip :type E_ToolShip%20Enum :default "NewEnumerator3"))
  ;[0.9723 1 0.2825] Tool unlocked
  (switch Utilities|FlowControl|Switch|SwitchonE_ToolShip ToolShip
    (:NewEnumerator0
      (Utilities|FlowControl|DoOnce false
        (:Completed
          (bind _current_widget (Variables|Private|Widget|GetCurrent%20Widget)
            (:then
              (Default|PlungerTutoVisibility _current_widget true)
              (Default|FirstTutoVisibility _current_widget false)
              (Utilities|FlowControl|Delay 1e+01)
              (bind _current_widget_2 (Variables|Private|Widget|GetCurrent%20Widget)
                (:then
                  (Default|PauseTutorial _current_widget_2)
                  (Default|PlungerTutorial _current_widget)
                  (Default|SetCurrentTarget (Variables|Default|GetBPC_Radar) (Utilities|Array|Get(acopy) (Variables|/Game/Blueprints/Game/Manager/BP_MicroArea_Manager.BP_MicroArea_Manager_C|GetParasitesInScene (Default|GetMicroArea (Private|GetValues|GetBPGameInstance) "NewEnumerator3")))))
                (:else)))
            (:else)))))))

(event Custom|ED_CatchFish
  (params (Area :type E_MicroZone%20Enum :default "NewEnumerator4") (Data :type S%20Creature%20Details%20Instanced%20Structure))
  ;[1 0.6052 0.4846] Fish Catch
  (if (Variables|Default|GetFirstTutorialActive)
    (Utilities|BranchFirstTuto 3
      (:True
        (Utilities|Map|Add (Variables|Private|Widget|Getb_FirstTuto) 3 true)
        (if (Utilities|Enum|Equal(Enum) (.CreatureName (Utilities|Struct|BreakS_CreatureDetailsInstanced Data)) "NewEnumerator16")
          (bind _current_widget (Variables|Private|Widget|GetCurrent%20Widget)
            (:then
              (Default|FirstTutorial _current_widget))
            (:else)))))))

(event Custom|PlayerInFlow
  ;[1 1 1] 2
  (if (Variables|Default|GetFirstTutorialActive)
    (Utilities|BranchFirstTuto 2
      (:True
        (Utilities|Map|Add (Variables|Private|Widget|Getb_FirstTuto) 2 true)
        (bind _current_widget (Variables|Private|Widget|GetCurrent%20Widget)
          (:then
            (Default|FirstTutorial _current_widget)
            (Default|ClearAllPings (Variables|Default|GetBPC_Radar))
            (Default|SetCurrentTarget (Variables|Default|GetBPC_Radar) (Default|GetMicroArea (Private|GetValues|GetBPGameInstance) "NewEnumerator3"))
            (Utilities|FlowControl|Delay 5.0)
            (bind _current_widget_2 (Variables|Private|Widget|GetCurrent%20Widget)
              (:then
                (Default|PauseTutorial _current_widget_2)
                (Default|FirstTutorial (Variables|Private|Widget|GetCurrent%20Widget))
                (Variables|Private|SetPingFish true)
                (Utilities|FlowControl|Delay 5.0)
                (bind _current_widget_3 (Variables|Private|Widget|GetCurrent%20Widget)
                  (:then
                    (Default|PauseTutorial _current_widget_3))
                  (:else)))
              (:else)))
          (:else))))))

(event Custom|ED_PlayerInMicroZone
  (params (MicroArea :type E_MicroZone%20Enum :default "NewEnumerator4"))
  ;[0.5431 1 0.6432] Player in micro zone
  (bind _current_widget (Variables|Private|Widget|GetCurrent%20Widget)
    (:then
      (Default|PlayerinZone _current_widget)
      (if (Variables|Private|GetPingFish)
        (switch Utilities|FlowControl|Switch|SwitchonE_MicroZone MicroArea
          (:NewEnumerator3
            (Default|ClearAllPings (Variables|Default|GetBPC_Radar))
            (Utilities|FlowControl|Delay 0.2)
            (for _array_element (Variables|/Game/Blueprints/Game/Manager/BP_CreatureManager.BP_CreatureManager_C|GetEntitiesAlive (Utilities|Array|Get(acopy) (Variables|/Game/Blueprints/Game/Manager/BP_MicroArea_Manager.BP_MicroArea_Manager_C|GetBP_CreatureManager (Default|GetMicroArea (Private|GetValues|GetBPGameInstance) MicroArea))))
              (Default|SetCurrentTarget (Variables|Default|GetBPC_Radar) _array_element)
              (Variables|Private|SetPingFish false))))))
    (:else)))

(event EventBeginPlay
  ;[0.968 1 0.441] Start
  (Utilities|FlowControl|Delay 0.2)
  (Utilities|Array|Clear (Variables|Private|Widget|GetListWidget))
  (Utilities|FlowControl|Sequence
    (:then_0
      (Private|Init|Initialisation))
    (:then_1
      (if (Variables|/Game/Blueprints/Data/Save/SaveSlot/BP_SaveSlot.BP_SaveSlot_C|GetActiveTutorial (Variables|/Game/Blueprints/Data/BP_GameInstance.BP_GameInstance_C|GetCurrentSaveSlot (Private|GetValues|GetBPGameInstance)))
        (Utilities|BranchFirstTuto
          (:True
            (private|Tutorial|TutorialInit)
            (Variables|Default|SetFirstTutorialActive true)
            (Utilities|FlowControl|Delay 2.0)
            (bind _current_widget (Variables|Private|Widget|GetCurrent%20Widget)
              (:then
                (Default|PauseTutorial _current_widget))
              (:else))))))))

(fn ConstructionScript)

(fn GetBPGameInstance
  (Variables|Private|GameInstance|GetGame%20Instance
    (:then
      _)
    (:else
      (bind _asbp_game_instance (Utilities|Casting|CastToBP_GameInstance (Game|GetGameInstance)))
      (Variables|Private|GameInstance|SetGame%20Instance _asbp_game_instance)))
  (return (Variables|Private|GameInstance|GetGame%20Instance)))

(fn Initialisation
  (bind _game_instance (Private|GetValues|GetBPGameInstance))
  (bind _game_instance_2 (Private|GetValues|GetBPGameInstance))
  (bind _game_instance_3 (Private|GetValues|GetBPGameInstance))
  (bind _player (Default|GetPlayer _game_instance_3))
  (Utilities|FlowControl|Sequence
    (:then_0
      ;[1 0.546 0.2172] Bind
      (EventDispatchers|BindEventtoEDonQuestCompleted _game_instance (EventDispatchers|CreateEvent :!event Custom|ED_QuestCompleted))
      (EventDispatchers|BindEventtoEDonUnlockToolManager (Variables|/Game/Blueprints/Game/Player/Controllers/BP_PlayerRefonte.BP_PlayerRefonte_C|GetBPC_ManagerTool (Default|GetPlayer _game_instance)) (EventDispatchers|CreateEvent :!event Custom|ED_ToolUnlock))
      (EventDispatchers|BindEventtoEDHaveCatchFish _game_instance (EventDispatchers|CreateEvent :!event Custom|ED_CatchFish))
      (EventDispatchers|BindEventtoEDPlayerinFlow _player (EventDispatchers|CreateEvent :!event Custom|PlayerInFlow))
      (EventDispatchers|BindEventtoEDPlayerIsMoving _player (EventDispatchers|CreateEvent :!event Custom|PlayerHaveMoveAndTurn))
      (EventDispatchers|BindEventtoEDPlayerChangeDirection _player (EventDispatchers|CreateEvent :!event Custom|PlayerHaveMoveAndTurn))
      (EventDispatchers|BindEventtoEDPlayerinMicroArea _game_instance_2 (EventDispatchers|CreateEvent :!event Custom|ED_PlayerInMicroZone))
      (EventDispatchers|BindEventtoEDPlayerExitMicroArea _game_instance_2 (EventDispatchers|CreateEvent :!event Custom|ED_PlayerExitMicroArea))
      (EventDispatchers|BindEventtoEDonOpen (Private|GetValues|GetSpaceport) (EventDispatchers|CreateEvent :!event Custom|ED_PlayerInSpaceport))
      (EventDispatchers|BindEventtoEDonClose (Private|GetValues|GetSpaceport) (EventDispatchers|CreateEvent :!event Custom|ED_SpaceportClose))
      (EventDispatchers|BindEventtoEDCinematicStarted (Private|GetValues|GetSpaceport) (EventDispatchers|CreateEvent :!event Custom|ED_CinematicSpaceportStarted))
      (EventDispatchers|BindEventtoEDonParasiteDestroyed (Default|GetMicroArea (Private|GetValues|GetBPGameInstance) "NewEnumerator3") (EventDispatchers|CreateEvent :!event Custom|ED_OnParasiteDestroyed)))
    (:then_1
      ;[0.2812 0.9901 1] Tools
      (Variables|Private|Tool|SetNetUnlocked (Private|GetValues|GetToolIsLocked "NewEnumerator2"))
      (Variables|Private|Tool|SetPlungeUnlocked (Private|GetValues|GetToolIsLocked "NewEnumerator0"))
      (Variables|Private|Tool|SetDashUnlocked (Private|GetValues|GetToolIsLocked "NewEnumerator4"))
      (Variables|Private|Tool|SetTeleportationUnlocked (Private|GetValues|GetToolIsLocked "NewEnumerator5")))
    (:then_2
      (bind _outactors (Actor|GetAllActorsOfClass "/Game/Blueprints/Game/Event/BP_PingActor.BP_PingActor_C"))
      (Variables|Private|Widget|SetPingActor _outactors)
      (Variables|/Game/Blueprints/Data/BP_GameInstance.BP_GameInstance_C|SetBP_Tutorial (Private|GetValues|GetBPGameInstance) self)
      (bind _outactors_2 (Actor|GetAllActorsOfClass "/Game/Blueprints/Game/Event/BP_TutoCollider.BP_TutoCollider_C"))
      (for _array_element _outactors_2
        (Utilities|Map|Add (Variables|Private|GetTutorialCollider) (Variables|/Game/Blueprints/Game/Event/BP_TutoCollider.BP_TutoCollider_C|GetTag _array_element) _array_element)
        (EventDispatchers|BindEventtoEDPlayerinZone _array_element (EventDispatchers|CreateEvent :!event Custom|ED_PlayerInTutorialZone))))))

(fn TutorialInit
  (bind _returnvalue (UserInterface|CreateWidget "/Game/Blueprints/Widgets/Tuto/UI_PopUpTuTo.UI_PopUpTuTo_C" 0 true false 0 0 0 "/Game/SFX/Sounds/NEW_OGG/Menu_UI_UX/Menu/SFX_ButtonHoveredMenu_Cue.SFX_ButtonHoveredMenu_Cue"))
  (UserInterface|Viewport|AddtoViewport _returnvalue 300)
  (Variables|Private|Widget|SetCurrent%20Widget _returnvalue)
  (Utilities|Map|Add (Variables|Private|Widget|Getb_FirstTuto) 0 true))

(fn InitWidgetToolUlockedWidget
  (params (Tool :type E_ToolShip%20Enum :default "NewEnumerator3")))

(fn GetToolIsLocked
  (params (Tool :type E_ToolShip%20Enum :default "NewEnumerator3"))
  (return (Utilities|Array|ContainsItem (Default|GetToolsUnlocked (Variables|/Game/Blueprints/Data/BP_GameInstance.BP_GameInstance_C|GetCurrentSaveSlot (Private|GetValues|GetBPGameInstance))) Tool)))

(fn IsFirstTimeCatched
  (params (S_CreatureDetailsInstanced :type S%20Creature%20Details%20Instanced%20Structure%20%28by%20ref%29))
  (return (Default|CreatureIsCaptured (Private|GetValues|GetBPGameInstance) (.CreatureName (Utilities|Struct|BreakS_CreatureDetailsInstanced S_CreatureDetailsInstanced)))))

(fn GetPingNear
  (params (UseTagFilter :type Boolean) (Tag :type Name))
  (for _array_element (Variables|Private|Widget|GetPingActor)
    (if UseTagFilter
      (if (Actor|ActorHasTag _array_element Tag)
        (if (>= (LocalVariables|GetDistance) (Transformation|GetDistanceTo (Game|Player|GetPlayerPawn 0) _array_element)) :!label _label
          (LocalVariables|SetDistance (Transformation|GetDistanceTo (Game|Player|GetPlayerPawn 0) _array_element))
          (LocalVariables|SetCurrentNearestPing _array_element)))
      (else
        (goto _label))))
  (LocalVariables|GetCurrentNearestPing
    (:then
      _)
    (:else
      (Development|PrintString "BP_Tutorial/GetPingNear : Output Empty")))
  (return (LocalVariables|GetCurrentNearestPing)))

(fn GetSpaceport
  (Variables|Private|GameInstance|GetBp%20Spaceport
    (:then
      _)
    (:else
      (bind _returnvalue (Actor|GetActorOfClass "/Game/Blueprints/Game/Environment/SpacePort/BP_SpacePort.BP_SpacePort_C"))
      (Variables|Private|GameInstance|SetBp%20Spaceport _returnvalue)))
  (return (Variables|Private|GameInstance|GetBp%20Spaceport)))

(fn IGetPriority
  (return 4))