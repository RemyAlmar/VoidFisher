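; Quest event for a breakable wall, apparently in the tutorial, that shatters when a dashing actor hits it head-on after all quests are completed.
; A valid hit enables auto-processing, switches the player camera to the event and destroys the tagged TutoWall collider.
; Processing swaps the static GeoMesh for the hidden Chaos geometry, triggers the master field and sets slow motion.
; Tick applies the target time dilation, which ActivateProcess restores after a delay.
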(event Custom|OnGeoHit_Event
  (params (SelfActor :type Actor%20Object%20Reference) (OtherActor :type Actor%20Object%20Reference) (NormalImpulse :type Vector) (Hit :type Hit%20Result%20Structure%20%28by%20ref%29))
  (bind _returnvalue (Actor|GetComponentbyClass OtherActor "/Game/Blueprints/AddOn/Components/BPC_Dash.BPC_Dash_C"))
  (if (CallFunction|HasAllQuestCompleted)
    (if (CallFunction|IsinOppositeDirection 0.75 (.ImpactNormal (Collision|BreakHitResult Hit)) (Transformation|GetActorForwardVector OtherActor))
      (Utilities|IsValid _returnvalue
        (:Is%20Valid
          (if (Variables|/Game/Blueprints/AddOn/Components/BPC_Dash.BPC_Dash_C|GetIsInDash _returnvalue)
            (CallFunction|SetAutoProcess true)
            (Default|NewCameraView (Default|GetPlayer (CallFunction|GetBPGameInstance)) self 1.0)
            (Actor|DestroyActor (Variables|Default|GetTutoColliderWall))))))))

(event EventActivateProcess
  (|CallParentFunction)
  (Utilities|FlowControl|Delay 2.0)
  (CallFunction|SetTargetTimeDilatation 1.0))

(event EventBeginPlay
  (Rendering|SetActorHiddenInGame (Variables|Default|GetGeoChaos) true)
  (CallFunction|Bind)
  (|CallParentFunction)
  (bind _outactors (Actor|GetAllActorswithTag "TutoWall"))
  (Variables|Default|SetTutoColliderWall (Utilities|Array|Get(acopy) _outactors)))

(event EventGameInstanceonQuestCompletedEvent
  (params (QuestName :type Name :default "None"))
  (if (CallFunction|HasAllQuestCompleted)
    _))

(event EventTick
  (params (DeltaSeconds :type Float%20%28single-precision%29))
  (CallFunction|SetTimeDilatation (Variables|Default|GetTargetTimeDilatation)))

(fn ConstructionScript
  (|CallParentFunction))

(fn Bind
  (bind _geomesh (Variables|Default|GetGeoMesh)
    (:then
      (Collision|BindEventtoOnActorHit _geomesh (EventDispatchers|CreateEvent :!event Custom|OnGeoHit_Event))
      (return))
    (:else)))

(fn Process
  (CallFunction|SetTargetTimeDilatation 0.2)
  (Rendering|SetActorHiddenInGame (Variables|Default|GetGeoChaos) false)
  (EventDispatchers|UnbindallEventsfromOnActorBeginOverlap (Variables|Default|GetGeoMesh))
  (Actor|DestroyActor (Variables|Default|GetGeoMesh))
  (Default|CETrigger (Variables|Default|GetFSMasterField))
  (|CallParentFunction))

(fn PreProcess
  (|CallParentFunction))