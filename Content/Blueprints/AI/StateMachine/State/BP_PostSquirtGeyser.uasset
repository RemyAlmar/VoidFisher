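; BP_PostSquirtGeyser is an AI state machine state that runs a geyser's post-squirt phase.
; On start it runs the parent logic and activates all of the geyser's particle systems.
; Cooldown updates call ChangeSize with the collider's capsule radius and half-height scaled by normalized time, with the change-direction flag set.
; When the cooldown resets, it switches the geyser to another state.
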(event EventEDonCooldownUpdateEvent
  (bind _returnvalue (CallFunction|GetNormalizedTime))
  (bind _bp_geyser (Variables|Default|GetBP_Geyser))
  (bind _collider (Variables|/Game/Blueprints/Game/Environment/Flow/BP_Geyser.BP_Geyser_C|GetCollider _bp_geyser))
  (Default|ChangeSize (Variables|Default|GetBP_Geyser) (* _returnvalue (Variables|/Script/Engine.CapsuleComponent|GetCapsuleRadius _collider)) (* _returnvalue (Variables|/Script/Engine.CapsuleComponent|GetCapsuleHalfHeight _collider)) true))

(event EventIStart
  (|CallParentFunction)
  (Default|ActiveAllParticleSystem (Variables|Default|GetBP_Geyser) true))

(event EventEDonCooldownResetEvent
  (CallFunction|IChangeState (Utilities|Enum|LiteralenumE_GeysersState "NewEnumerator3")))