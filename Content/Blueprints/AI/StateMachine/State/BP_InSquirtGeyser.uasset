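; Geyser state machine state for the squirt phase, which animates the geyser's size while a cooldown runs.
; Start, update and quit defer to the parent state.
; Each cooldown update resizes BPGeyser at its active radius, with half height scaled by normalized time and no direction change.
; When the cooldown resets, it switches to another geyser state.
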(event EventIStart
  (|CallParentFunction))

(event EventIUpdate
  (params (DeltaSeconds :type Float%20%28double-precision%29))
  (|CallParentFunction DeltaSeconds))

(event EventIQuit
  (|CallParentFunction))

(event EventEDonCooldownResetEvent
  (CallFunction|IChangeState (Utilities|Enum|LiteralenumE_GeysersState "NewEnumerator1")))

(event EventEDonCooldownUpdateEvent
  (bind _bp_geyser (Variables|Default|GetBP_Geyser))
  (Default|ChangeSize _bp_geyser (Variables|/Game/Blueprints/Game/Environment/Flow/BP_Geyser.BP_Geyser_C|GetRadiusActive _bp_geyser) (* (CallFunction|GetNormalizedTime) (Variables|/Game/Blueprints/Game/Environment/Flow/BP_Geyser.BP_Geyser_C|GetHalfHeightActive _bp_geyser)) false))