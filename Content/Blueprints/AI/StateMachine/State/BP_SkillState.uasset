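; AI state machine state that serves as a base for a skill with a cooldown, leaving most event hooks empty.
; Each update fires the skill-unused event while the skill is available or usable, and otherwise advances an auto-resetting cooldown timer.
; Cooldown start, update and reset are relayed through event dispatchers.
; UseSkill clears the usable flag, and the flag setters have change events for reacting to new values.
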(event Custom|OnSkillAvailableChanged_Event
  (params (SkillAvailable :type Boolean)))

(event Custom|WhileSkillUnused_Event
  (params (DeltaTime :type Float%20%28double-precision%29))
  ;[1 1 1] Si laissé alors fais le truc à l'infini
)

(event Custom|OnCanUseValueChanged_Event
  (params (CanUseSkill :type Boolean)))

(event EventIStart)

(event EventIQuit)

(event EventEDonCooldownResetEvent
  (CallFunction|SetStartCooldown false)
  (Default|CallEDonCooldownReset))

(event EventIUpdate
  (params (DeltaSeconds :type Float%20%28double-precision%29))
  (if (Variables|Default|GetSkillAvailable)
    (CallFunction|WhileSkillUnusedEvent DeltaSeconds :!label _label)
    (elif (Variables|Default|GetCanUseSkill)
      (goto _label)
      (elif (CallFunction|TimerPos (Variables|Default|GetCurrentTime) DeltaSeconds (Variables|Default|GetCooldownMax) true)
        (CallFunction|EDonCooldownResetEvent)
        (else
          (CallFunction|SetStartCooldown true)
          (CallFunction|EDonCooldownUpdateEvent DeltaSeconds))))))

(event EventEDonCooldownUpdateEvent
  (params (DeltaTime :type Float%20%28double-precision%29))
  (Default|CallEDonCooldownUpdate))

(event EventEDonCooldownStartEvent
  (Default|CallEDonCooldownStart))

(fn UseSkill
  (CallFunction|SetCanUseSkill false))

(fn SetCanUseSkill
  (params (CanUseSkill :type Boolean))
  (LocalVariables|SetPreviousValue (Variables|Default|GetCanUseSkill))
  (Variables|Default|SetCanUseSkill CanUseSkill)
  (if (!= (Variables|Default|GetCanUseSkill) (LocalVariables|GetPreviousValue))
    (CallFunction|OnCanUseValueChangedEvent (Variables|Default|GetCanUseSkill))))

(fn SetSkillAvailable
  (params (SkillAvailable :type Boolean))
  (LocalVariables|SetPreviousValue (Variables|Default|GetSkillAvailable))
  (Variables|Default|SetSkillAvailable SkillAvailable)
  (if (!= (Variables|Default|GetSkillAvailable) (LocalVariables|GetPreviousValue))
    (CallFunction|OnSkillAvailableChangedEvent (Variables|Default|GetSkillAvailable))))