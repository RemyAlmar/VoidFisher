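; AI state machine state that runs a repeating cooldown timer while it updates.
; InitState reads the cooldown length from the Commander's ListCooldown map, keyed by the state's enum name.
; Each IUpdate calls the parent, then advances the timer via TimerPos, firing the reset dispatcher on expiry and the update dispatcher otherwise.
; The timer auto-resets to zero on expiry, while IStart and IQuit leave it untouched.
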(event Custom|ED_OnCooldownReset_Event
  (Default|CallEDonCooldownReset))

(event Custom|ED_OnCooldownUpdate_Event
  (Default|CallEDonCooldownUpdate))

(event EventIStart)

(event EventIUpdate
  (params (DeltaSeconds :type Float%20%28double-precision%29))
  (|CallParentFunction DeltaSeconds)
  (if (CallFunction|TimerPos (Variables|Default|GetCurrentTime) DeltaSeconds (Variables|Default|GetCooldownMax) true)
    (CallFunction|EDonCooldownResetEvent)
    (else
      (CallFunction|EDonCooldownUpdateEvent))))

(event EventIQuit)

(fn InitState
  (params (Target :type Actor%20Object%20Reference) (StateName :type Byte :default 0) (Commander :type BP%20State%20Commander%20Object%20Reference))
  (|CallParentFunction Target StateName Commander)
  (Variables|Default|SetCooldownMax (.Value (Utilities|Map|Find (Variables|/Game/Blueprints/AI/StateMachine/BP_StateCommander.BP_StateCommander_C|GetListCooldown Commander) (Variables|Default|GetEStateName)))))

(fn TimerPos
  (params (CurrentTime :type Float%20%28double-precision%29%20%28by%20ref%29) (DeltaTime :type Float%20%28double-precision%29) (MaxTime :type Float%20%28double-precision%29) (AutoReset :type Boolean))
  (bind _output_get (LocalVariables|SetFutureTime (+ CurrentTime DeltaTime)))
  (bind _output_get_2 (LocalVariables|SetTimeReached (>= _output_get MaxTime)))
  (if _output_get_2
    (if AutoReset
      (LocalVariables|SetFutureTime 0.0)
      (else
        (LocalVariables|SetFutureTime MaxTime))))
  (|SetBy-RefVar (Variables|Default|GetCurrentTime) (LocalVariables|GetFutureTime))
  (return (LocalVariables|GetTimeReached)))