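; BP_QuitGeyser is a state in a geyser state machine that handles the geyser's quit phase.
; Start, update and quit call the parent state's logic and print debug text.
; Cooldown updates call ChangeSize on the geyser with its base radius and half-height and the change-direction flag set.
; The cooldown reset event switches the machine to another geyser state.
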(event EventIStart
  (|CallParentFunction)
  (Development|PrintText 0 "Start Quit Geyser" true true "(R=1.000000,G=0.000000,B=0.058054,A=1.000000)" 3.0))

(event EventIUpdate
  (params (DeltaSeconds :type Float%20%28double-precision%29))
  (|CallParentFunction DeltaSeconds)
  (Development|PrintText 0 "Update Quit Geyser" true true "(R=1.000000,G=0.000000,B=0.058054,A=1.000000)" 0.0))

(event EventIQuit
  (|CallParentFunction)
  (Development|PrintText 0 "Quit Quit Geyser" true true "(R=1.000000,G=0.000000,B=0.058054,A=1.000000)" 3.0))

(event EventEDonCooldownResetEvent
  (CallFunction|IChangeState (Utilities|Enum|LiteralenumE_GeysersState "NewEnumerator3")))

(event EventEDonCooldownUpdateEvent
  (bind _bp_geyser (Variables|Default|GetBP_Geyser))
  (Default|ChangeSize _bp_geyser (Variables|/Game/Blueprints/Game/Environment/Flow/BP_Geyser.BP_Geyser_C|GetRadiusBase _bp_geyser) (Variables|/Game/Blueprints/Game/Environment/Flow/BP_Geyser.BP_Geyser_C|GetHalfHeightBase _bp_geyser) true))