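; BP_State is the base state for an AI state machine, with empty start, update and quit interface events.
; InitState stores the target, the state's enum name and the Commander, to which state change requests are forwarded.
; GetComponentInstance returns the target's component of a given class, adding one at runtime if none exists.
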(event EventIStart)

(event EventIUpdate
  (params (DeltaSeconds :type Float%20%28double-precision%29)))

(event EventIQuit)

(event EventIChangeState
  (params (TargetState :type Byte :default 0))
  (Default|IChangeState (Variables|Default|GetCommander) TargetState))

(fn InitState
  (params (Target :type Actor%20Object%20Reference) (StateName :type Byte) (Commander :type BP%20State%20Commander%20Object%20Reference))
  (Variables|Default|SetTarget Target)
  (Variables|Default|SetEStateName StateName)
  (Variables|Default|SetCommander Commander))

(fn GetComponentInstance
  (params (Target :type Actor%20Object%20Reference) (ClassComponent :type Actor%20Component%20Class%20Reference))
  (LocalVariables|SetCurrentActorComp (Actor|GetComponentbyClass Target ClassComponent))
  (Utilities|IsValid (LocalVariables|GetCurrentActorComp)
    (:Is%20Valid
      _)
    (:Is%20Not%20Valid
      (bind _returnvalue (Game|AddComponentbyClass Target ClassComponent))
      (LocalVariables|SetCurrentActorComp _returnvalue)))
  (return (LocalVariables|GetCurrentActorComp)))