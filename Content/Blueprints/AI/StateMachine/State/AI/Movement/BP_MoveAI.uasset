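; BP_MoveAI is the AI movement state in the creature state machine, driving locomotion through the creature's physics movement component.
; On start it enables physics at neutral speed, then each update sets rotation rate by speed, moves the creature along its forward vector and applies rotation.
; InitState binds a reset-speed event that picks a neutral, hunter or prey target speed from whether the creature is quiet or has prey in range.
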(event Custom|Owner_ED_ResetSpeed_Event
  (bind _selfcreature (Variables|Default|GetSelfCreature))
  (bind _selfcreature_2 (Variables|Default|GetSelfCreature))
  (bind _value (Default|GetAIData _selfcreature_2))
  (bind _speedms (Utilities|Struct|BreakS_AICreatureBehaviorSettings _value))
  (if (Default|IsQuiet _selfcreature_2)
    (Variables|/Game/Blueprints/AI/Pawn/BP_CreatureGeneric.BP_CreatureGeneric_C|SetTargetTempSpeed _selfcreature_2 (.neutre _speedms))
    (elif (Default|HasPreyinRange (Variables|/Game/Blueprints/AI/Pawn/BP_CreatureGeneric.BP_CreatureGeneric_C|GetBPC_Predator _selfcreature_2))
      (Variables|/Game/Blueprints/AI/Pawn/BP_CreatureGeneric.BP_CreatureGeneric_C|SetTargetTempSpeed _selfcreature (.hunter _speedms))
      (else
        (Variables|/Game/Blueprints/AI/Pawn/BP_CreatureGeneric.BP_CreatureGeneric_C|SetTargetTempSpeed _selfcreature (.prey _speedms))))))

(event EventIStart
  (bind _selfcreature (Variables|Default|GetSelfCreature))
  (Default|On/OffPhysics (Variables|/Game/Blueprints/AI/Pawn/BP_CreatureGeneric.BP_CreatureGeneric_C|GetBPC_ActorPhysicsMovement _selfcreature) true (Utilities|Struct|BreakS_FloatCreatureMode (Utilities|Struct|BreakS_AICreatureBehaviorSettings (Utilities|Struct|BreakS_CreatureDetailsInstanced (Variables|/Game/Blueprints/AI/Pawn/BP_CreatureGeneric.BP_CreatureGeneric_C|GetUserData _selfcreature)))))
  (|CallParentFunction))

(event EventIUpdate
  (params (DeltaSeconds :type Float%20%28double-precision%29))
  (bind _selfcreature (Variables|Default|GetSelfCreature))
  (bind _bpc_actorphysicsmovement (Variables|/Game/Blueprints/AI/Pawn/BP_CreatureGeneric.BP_CreatureGeneric_C|GetBPC_ActorPhysicsMovement _selfcreature))
  (Default|SetRotationRatebySpeed (Variables|/Game/Blueprints/AI/Pawn/BP_CreatureGeneric.BP_CreatureGeneric_C|GetBPC_ActorPhysicsMovement (Variables|Default|GetSelfCreature)))
  (Default|ApplyMovement _bpc_actorphysicsmovement (Transformation|GetActorForwardVector _selfcreature))
  (Default|ApplyRotation _bpc_actorphysicsmovement)
  (|CallParentFunction DeltaSeconds))

(event EventIQuit
  (|CallParentFunction))

(fn InitState
  (params (Target :type Actor%20Object%20Reference) (StateName :type Byte :default 0) (Commander :type BP%20State%20Commander%20Object%20Reference))
  (|CallParentFunction Target StateName Commander)
  (EventDispatchers|BindEventtoEDResetSpeed (Variables|Default|GetSelfCreature) (EventDispatchers|CreateEvent :!event OwnerEDResetSpeedEvent)))