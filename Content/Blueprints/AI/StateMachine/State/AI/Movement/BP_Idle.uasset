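; BP_Idle is the idle movement state in the AI creature state machine.
; On start it tells the creature's BPCActorPhysicsMovement component to stop speed.
; Each update still applies rotation and movement along the creature's forward vector through that component.
; Start, update and quit all chain to the parent state, and quit adds no logic of its own.
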(event EventIStart
  (Default|StopSpeed (Variables|/Game/Blueprints/AI/Pawn/BP_CreatureGeneric.BP_CreatureGeneric_C|GetBPC_ActorPhysicsMovement (Variables|Default|GetSelfCreature)))
  (|CallParentFunction))

(event EventIUpdate
  (params (DeltaSeconds :type Float%20%28double-precision%29))
  (bind _selfcreature (Variables|Default|GetSelfCreature))
  (bind _bpc_actorphysicsmovement (Variables|/Game/Blueprints/AI/Pawn/BP_CreatureGeneric.BP_CreatureGeneric_C|GetBPC_ActorPhysicsMovement _selfcreature))
  (Default|ApplyRotation _bpc_actorphysicsmovement)
  (Default|ApplyMovement _bpc_actorphysicsmovement (Transformation|GetActorForwardVector _selfcreature))
  (|CallParentFunction DeltaSeconds))

(event EventIQuit
  (|CallParentFunction))