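; AI movement state that holds a creature stunned while active.
; On start it zeroes target speed, deactivates the skill and detection state managers, fires the creature's stunned event and attaches a stun Niagara effect bound to its skeletal mesh.
; Each update applies zero movement.
; On quit it restores neutral speed from AI data, reactivates both managers and destroys the effect.
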(event EventIStart
  (bind _selfcreature (Variables|Default|GetSelfCreature))
  (bind _selfcreature_2 (Variables|Default|GetSelfCreature))
  (bind _skm_creature (Variables|/Game/Blueprints/AI/Pawn/BP_CreatureGeneric.BP_CreatureGeneric_C|GetSKM_Creature _selfcreature))
  (|CallParentFunction)
  (Variables|/Game/Blueprints/AddOn/Components/BPC_ActorPhysicsMovement.BPC_ActorPhysicsMovement_C|SetTargetSpeed (Variables|/Game/Blueprints/AI/Pawn/BP_CreatureGeneric.BP_CreatureGeneric_C|GetBPC_ActorPhysicsMovement _selfcreature_2) 0.0)
  (Components|Activation|Deactivate (Variables|/Game/Blueprints/AI/Pawn/BP_CreatureGeneric.BP_CreatureGeneric_C|GetBPC_StateManager_Skills _selfcreature_2))
  (Components|Activation|Deactivate (Variables|/Game/Blueprints/AI/Pawn/BP_CreatureGeneric.BP_CreatureGeneric_C|GetBPC_StateManager_Detection _selfcreature_2))
  (Default|EDonStunnedEvent (Variables|Default|GetSelfCreature))
  (bind _returnvalue (Niagara|SpawnSystemAttached "/Game/VFX/Niagara/Fish/NS_Stunned.NS_Stunned" _skm_creature "None" "0, 0, 0" "0, 0, 0" "SnapToTargetIncludingScale" false))
  (Class|NiagaraComponent|SetVariableObject _returnvalue "SKM_Niagara" _skm_creature)
  (Variables|Default|SetNS_Stunned _returnvalue))

(event EventIQuit
  (bind _selfcreature (Variables|Default|GetSelfCreature))
  (|CallParentFunction)
  (Variables|/Game/Blueprints/AddOn/Components/BPC_ActorPhysicsMovement.BPC_ActorPhysicsMovement_C|SetTargetSpeed (Variables|/Game/Blueprints/AI/Pawn/BP_CreatureGeneric.BP_CreatureGeneric_C|GetBPC_ActorPhysicsMovement _selfcreature) (.neutre (Utilities|Struct|BreakS_AICreatureBehaviorSettings (Default|GetAIData _selfcreature))))
  (Components|Activation|Activate (Variables|/Game/Blueprints/AI/Pawn/BP_CreatureGeneric.BP_CreatureGeneric_C|GetBPC_StateManager_Skills _selfcreature) false)
  (Components|Activation|Activate (Variables|/Game/Blueprints/AI/Pawn/BP_CreatureGeneric.BP_CreatureGeneric_C|GetBPC_StateManager_Detection _selfcreature) false)
  (bind _ns_stunned (Variables|Default|GetNS_Stunned)
    (:then
      (Components|DestroyComponent _ns_stunned))
    (:else)))

(event EventIUpdate
  (params (DeltaSeconds :type Float%20%28double-precision%29))
  (Default|ApplyMovement (Variables|/Game/Blueprints/AI/Pawn/BP_CreatureGeneric.BP_CreatureGeneric_C|GetBPC_ActorPhysicsMovement (Variables|Default|GetSelfCreature)) "0, 0, 0")
  (|CallParentFunction DeltaSeconds))