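; AI state for a parasited creature, which lasts until every parasite attached to it is destroyed.
; On init it spawns parasites on anchor sockets, makes the creature's sight ignore them and the player, and adds an overlay material and Niagara effect.
; Destroy bindings track remaining parasites; the last one fires the creature's destroy dispatcher and swaps effects.
; Update then eases the overlay's Dissolve parameter out, with a debug print.
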(event Custom|ED_OnParasiteDestroyed_Event
  (params (DestroyedActor :type Actor%20Object%20Reference))
  (bind _selfcreature (Variables|Default|GetSelfCreature))
  (bind _selfcreature_2 (Variables|Default|GetSelfCreature))
  (bind _parasite (Variables|Default|GetParasite))
  (if (Utilities|Array|ContainsItem (Variables|Default|GetParasite) DestroyedActor)
    (Game|UnbindEventfromOnDestroyed DestroyedActor (EventDispatchers|CreateEvent :!event Custom|ED_OnParasiteDestroyed_Event))
    (Utilities|Array|RemoveItem _parasite DestroyedActor)
    (if (Utilities|Array|IsEmpty _parasite)
      (Default|CallEDonDestroyActor _selfcreature_2 _selfcreature_2)
      (bind _ns_parasited (Variables|Default|GetNS_Parasited)
        (:then
          (Components|DestroyComponent _ns_parasited))
        (:else
          _))
      (Niagara|SpawnSystemAttached (Variables|/Game/Blueprints/AI/Pawn/BP_CreatureGeneric.BP_CreatureGeneric_C|GetNiagara%20System _selfcreature) (Variables|/Game/Blueprints/AI/Pawn/BP_CreatureGeneric.BP_CreatureGeneric_C|GetSKM_Creature _selfcreature) "None" "0, 0, 0" "0, 0, 0" "SnapToTarget" false true "AutoRelease"))))

(event EventIUpdate
  (params (DeltaSeconds :type Float%20%28double-precision%29))
  (|CallParentFunction DeltaSeconds)
  (if (Utilities|Array|IsEmpty (Variables|Default|GetParasite))
    (bind _dmi_parasiteoverride (Variables|Private|Material|GetDMI_ParasiteOverride)
      (:then
        (Variables|Private|Material|SetDissolve (Math|Interpolation|FInterpTo (Variables|Private|Material|GetDissolve) -1.0 DeltaSeconds 1.0))
        (Rendering|Material|SetScalarParameterValue _dmi_parasiteoverride "Dissolve" (Math|Interpolation|FInterpTo (Variables|Private|Material|GetDissolve) -1.0 DeltaSeconds 1.0) :!class /Script/Engine.MaterialInstanceDynamic)
        (Development|PrintText 0 (Utilities|Text|FormatText "Dissolve {A}" (Math|Interpolation|FInterpTo (Variables|Private|Material|GetDissolve) -1.0 DeltaSeconds 1.0)) true true "(R=1.000000,G=0.021949,B=0.000000,A=1.000000)"))
      (:else))))

(fn InitState
  (params (Target :type Actor%20Object%20Reference) (StateName :type Byte :default 0) (Commander :type BP%20State%20Commander%20Object%20Reference))
  (bind _selfcreature (Variables|Default|GetSelfCreature))
  (bind _selfcreature_2 (Variables|Default|GetSelfCreature))
  (bind _actorsignoredtosee (Variables|/Game/Blueprints/AI/Pawn/BP_CreatureGeneric.BP_CreatureGeneric_C|GetActorsIgnoredToSee _selfcreature))
  (bind _skm_creature (Variables|/Game/Blueprints/AI/Pawn/BP_CreatureGeneric.BP_CreatureGeneric_C|GetSKM_Creature _selfcreature_2))
  (|CallParentFunction Target StateName Commander)
  (Utilities|FlowControl|Sequence
    (:then_0
      (bind _returnvalue (Default|SpawnSomethingonSocket _selfcreature "/Game/Blueprints/AI/Pawn/BP_ParasiteToAnchored.BP_ParasiteToAnchored_C" "AnchorParasite_Socket"))
      (bind _output_get (Variables|Default|SetParasite _returnvalue))
      (Utilities|Array|AppendArray _actorsignoredtosee _output_get)
      (Utilities|Array|Add _actorsignoredtosee (Default|GetPlayer (Default|GetBPGameInstance _selfcreature)))
      (for _array_element (Variables|Default|GetParasite)
        (Game|BindEventtoOnDestroyed _array_element (EventDispatchers|CreateEvent :!event Custom|ED_OnParasiteDestroyed_Event))))
    (:then_1
      (bind _returnvalue_2 (Rendering|Material|CreateDynamicMaterialInstance (Variables|Default|GetSelfCreature) "/Game/VFX/Materials/Fish/M_ParasitedOverlay.M_ParasitedOverlay" "None" :!class /Script/Engine.KismetMaterialLibrary))
      (bind _output_get_2 (Variables|Private|Material|SetDMI_ParasiteOverride _returnvalue_2))
      (Rendering|Material|SetOverlayMaterial _skm_creature _output_get_2 :!class /Script/Engine.MeshComponent)
      (bind _returnvalue_3 (Niagara|SpawnSystemAttached "/Game/VFX/Niagara/Fish/NS_FishParasited.NS_FishParasited" _skm_creature "None" "0, 0, 0" "0, 0, 0" "SnapToTarget" false))
      (Variables|Default|SetNS_Parasited _returnvalue_3))))