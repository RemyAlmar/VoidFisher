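; Base AI state for prey creatures that adjusts movement in response to predators.
; On init it binds to the creature's BPCPrey dispatchers, and on start it adds and starts a BP_DetectForward state in the detection state manager.
; Reacting to a predator applies Prey rotation rate and target speed from AI data; losing all predators restores Neutre values if the creature is quiet.
; The predator-out, in-range and aimed handlers are empty.
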(event Custom|Prey_ED_IsWithoutPredator
  (if (Default|IsQuiet (Variables|Default|GetSelfCreature))
    (CallFunction|SetNeutralRotationRateandSpeed)))

(event Custom|Prey_ED_ReactOnPredator_Out
  (params (TargetPredator :type Actor%20Object%20Reference)))

(event Custom|Prey_ED_SeePredatorInRange)

(event Custom|Prey_ED_IsAimed)

(event Custom|Prey_ED_ReactOnPredator_In
  (params (TargetPredator :type Actor%20Object%20Reference))
  (CallFunction|SetPreyRotationRateandSpeed))

(event EventIStart
  (|CallParentFunction)
  (Default|AddState (Variables|/Game/Blueprints/AI/Pawn/BP_CreatureGeneric.BP_CreatureGeneric_C|GetBPC_StateManager_Detection (Variables|Default|GetSelfCreature)) (Utilities|Enum|LiteralenumE_StateDetection "NewEnumerator0") true "/Game/Blueprints/AI/StateMachine/State/AI/Detection/BP_DetectForward.BP_DetectForward_C"))

(fn InitState
  (params (Target :type Actor%20Object%20Reference) (StateName :type Byte :default 0) (Commander :type BP%20State%20Commander%20Object%20Reference))
  (bind _selfcreature (Variables|Default|GetSelfCreature))
  (bind _bpc_prey (Variables|/Game/Blueprints/AI/Pawn/BP_CreatureGeneric.BP_CreatureGeneric_C|GetBPC_Prey _selfcreature))
  (|CallParentFunction Target StateName Commander)
  (EventDispatchers|BindEventtoEDReactonPredatorin _bpc_prey (EventDispatchers|CreateEvent :!event Custom|Prey_ED_ReactOnPredator_In))
  (EventDispatchers|BindEventtoEDReactonPredatorOut _bpc_prey (EventDispatchers|CreateEvent :!event Custom|Prey_ED_ReactOnPredator_Out))
  (EventDispatchers|BindEventtoEDSeePredatorinRange _bpc_prey (EventDispatchers|CreateEvent :!event Custom|Prey_ED_SeePredatorInRange))
  (EventDispatchers|BindEventtoEDIsAimed _bpc_prey (EventDispatchers|CreateEvent :!event Custom|Prey_ED_IsAimed))
  (EventDispatchers|BindEventtoEDIsWithoutPredator _bpc_prey (EventDispatchers|CreateEvent :!event Custom|Prey_ED_IsWithoutPredator)))

(fn SetPreyRotationRateandSpeed
  (bind _selfcreature (Variables|Default|GetSelfCreature))
  (bind _value (Default|GetAIData _selfcreature))
  (bind _bpc_actorphysicsmovement (Variables|/Game/Blueprints/AI/Pawn/BP_CreatureGeneric.BP_CreatureGeneric_C|GetBPC_ActorPhysicsMovement _selfcreature))
  (bind (_rotationratedegs _speedms) (Utilities|Struct|BreakS_AICreatureBehaviorSettings _value))
  (Variables|/Game/Blueprints/AddOn/Components/BPC_ActorPhysicsMovement.BPC_ActorPhysicsMovement_C|SetRotationRate _bpc_actorphysicsmovement (.prey _rotationratedegs))
  (Variables|/Game/Blueprints/AddOn/Components/BPC_ActorPhysicsMovement.BPC_ActorPhysicsMovement_C|SetTargetSpeed _bpc_actorphysicsmovement (.prey _speedms))
  (return))

(fn SetNeutralRotationRateandSpeed
  (bind _selfcreature (Variables|Default|GetSelfCreature))
  (bind _value (Default|GetAIData _selfcreature))
  (bind _bpc_actorphysicsmovement (Variables|/Game/Blueprints/AI/Pawn/BP_CreatureGeneric.BP_CreatureGeneric_C|GetBPC_ActorPhysicsMovement _selfcreature))
  (bind (_rotationratedegs _speedms) (Utilities|Struct|BreakS_AICreatureBehaviorSettings _value))
  (Variables|/Game/Blueprints/AddOn/Components/BPC_ActorPhysicsMovement.BPC_ActorPhysicsMovement_C|SetRotationRate _bpc_actorphysicsmovement (.neutre _rotationratedegs))
  (Variables|/Game/Blueprints/AddOn/Components/BPC_ActorPhysicsMovement.BPC_ActorPhysicsMovement_C|SetTargetSpeed _bpc_actorphysicsmovement (.neutre _speedms))
  (return))