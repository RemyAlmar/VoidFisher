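; BP_DetectForward is an AI detection state in a creature state machine that checks each update whether the creature can move forward.
; When forward movement is possible and the creature is quiet, it has a one percent chance per update to switch to another detection state.
; When forward movement is blocked, it switches to a different detection state.
; Both switches require the commander to have the target state, and start, update and quit call their parent implementations.
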(event EventIStart
  (|CallParentFunction))

(event EventIUpdate
  (params (DeltaSeconds :type Float%20%28double-precision%29))
  (bind _returnvalue (Utilities|Enum|LiteralenumE_StateDetection "NewEnumerator4"))
  (bind _returnvalue_2 (Utilities|Enum|LiteralenumE_StateDetection "NewEnumerator7"))
  (bind _selfcreature (Variables|Default|GetSelfCreature))
  (if (Default|CanMoveForward _selfcreature)
    (if (Default|IsQuiet _selfcreature)
      (if (Math|Random|RandomBoolwithWeight 0.01)
        (if (Default|HasState (Variables|Default|GetCommander) _returnvalue_2)
          (CallFunction|IChangeState _returnvalue_2))))
    (elif (Default|HasState (Variables|Default|GetCommander) _returnvalue)
      (CallFunction|IChangeState _returnvalue)))
  (|CallParentFunction DeltaSeconds))

(event EventIQuit
  (|CallParentFunction))