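; BP_PredatorFollowConstantly is an AI detection state that steers a predator creature toward its prey.
; When the have-to-hunt event fires, it calls the parent, then copies the prey direction from the creature's predator component into the target direction of its physics movement component.
; The add-prey, remove-prey and without-prey events only forward to the parent class.
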(event EventPredatorEDAddPreytoHuntEvent
  (params (PreyToHunt :type Actor%20Object%20Reference))
  (|CallParentFunction PreyToHunt))

(event EventPredatorEDHavetoHuntEvent
  (bind _selfcreature (Variables|Default|GetSelfCreature))
  (|CallParentFunction)
  (Variables|/Game/Blueprints/AddOn/Components/BPC_ActorPhysicsMovement.BPC_ActorPhysicsMovement_C|SetTargetDirection (Variables|/Game/Blueprints/AI/Pawn/BP_CreatureGeneric.BP_CreatureGeneric_C|GetBPC_ActorPhysicsMovement _selfcreature) (Default|GetPreyDirection (Variables|/Game/Blueprints/AI/Pawn/BP_CreatureGeneric.BP_CreatureGeneric_C|GetBPC_Predator _selfcreature))))

(event EventPredatorEDIsWithoutPrey
  (|CallParentFunction))

(event EventPredatorEDRemovePreytoHuntEvent
  (params (PreyToRemoveFromHunt :type Actor%20Object%20Reference))
  (|CallParentFunction PreyToRemoveFromHunt))