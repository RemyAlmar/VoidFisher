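; Base AI state for predator creatures that switches movement between hunting and neutral profiles.
; On start it adds and starts a forward-detection state on the creature's detection state manager.
; InitState binds to the predator component's hunt events: adding prey applies Hunter rotation rate and speed from creature behavior settings.
; Losing all prey restores Neutre values if the creature is quiet; the other two hunt handlers are empty.
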(event Custom|Predator_ED_IsWithoutPrey
  (if (Default|IsQuiet (Variables|Default|GetSelfCreature))
    (CallFunction|SetNeutralRotationRateandSpeed)))

(event Custom|Predator_ED_HaveToHunt_Event)

(event Custom|Predator_ED_RemovePreyToHunt_Event
  (params (PreyToRemoveFromHunt :type Actor%20Object%20Reference)))

(event Custom|Predator_ED_AddPreyToHunt_Event
  (params (PreyToHunt :type Actor%20Object%20Reference))
  (CallFunction|SetRotationRateandSpeed))

(event EventIStart
  (|CallParentFunction)
  (Default|AddState (Variables|/Game/Blueprints/AI/Pawn/BP_CreatureGeneric.BP_CreatureGeneric_C|GetBPC_StateManager_Detection (Variables|Default|GetSelfCreature)) (Utilities|Enum|LiteralenumE_StateDetection "NewEnumerator0") true "/Game/Blueprints/AI/StateMachine/State/AI/Detection/BP_DetectForward.BP_DetectForward_C"))

(fn InitState
  (params (Target :type Actor%20Object%20Reference) (StateName :type Byte :default 0) (Commander :type BP%20State%20Commander%20Object%20Reference))
  (bind _selfcreature (Variables|Default|GetSelfCreature))
  (bind _bpc_predator (Variables|/Game/Blueprints/AI/Pawn/BP_CreatureGeneric.BP_CreatureGeneric_C|GetBPC_Predator _selfcreature))
  (|CallParentFunction Target StateName Commander)
  (EventDispatchers|BindEventtoEDAddPreytoHunt _bpc_predator (EventDispatchers|CreateEvent :!event Custom|Predator_ED_AddPreyToHunt_Event))
  (EventDispatchers|BindEventtoEDHavetoHunt _bpc_predator (EventDispatchers|CreateEvent :!event Custom|Predator_ED_HaveToHunt_Event))
  (EventDispatchers|BindEventtoEDRemovePreytoHunt _bpc_predator (EventDispatchers|CreateEvent :!event Custom|Predator_ED_RemovePreyToHunt_Event))
  (EventDispatchers|BindEventtoEDIsWithoutPrey _bpc_predator (EventDispatchers|CreateEvent :!event Custom|Predator_ED_IsWithoutPrey)))

(fn SetRotationRateandSpeed
  (bind _selfcreature (Variables|Default|GetSelfCreature))
  (bind _userdata (Variables|/Game/Blueprints/AI/Pawn/BP_CreatureGeneric.BP_CreatureGeneric_C|GetUserData _selfcreature))
  (bind _bpc_actorphysicsmovement (Variables|/Game/Blueprints/AI/Pawn/BP_CreatureGeneric.BP_CreatureGeneric_C|GetBPC_ActorPhysicsMovement _selfcreature))
  (bind _creaturebehaviorsettings (Utilities|Struct|BreakS_CreatureDetailsInstanced _userdata))
  (bind (_rotationratedegs _speedms) (Utilities|Struct|BreakS_AICreatureBehaviorSettings _creaturebehaviorsettings))
  (Variables|/Game/Blueprints/AddOn/Components/BPC_ActorPhysicsMovement.BPC_ActorPhysicsMovement_C|SetRotationRate _bpc_actorphysicsmovement (.Hunter (Utilities|Struct|BreakS_FloatCreatureMode _rotationratedegs)))
  (Variables|/Game/Blueprints/AddOn/Components/BPC_ActorPhysicsMovement.BPC_ActorPhysicsMovement_C|SetTargetSpeed _bpc_actorphysicsmovement (.Hunter (Utilities|Struct|BreakS_FloatCreatureMode _speedms))))

(fn SetNeutralRotationRateandSpeed
  (bind _selfcreature (Variables|Default|GetSelfCreature))
  (bind _userdata (Variables|/Game/Blueprints/AI/Pawn/BP_CreatureGeneric.BP_CreatureGeneric_C|GetUserData _selfcreature))
  (bind _bpc_actorphysicsmovement (Variables|/Game/Blueprints/AI/Pawn/BP_CreatureGeneric.BP_CreatureGeneric_C|GetBPC_ActorPhysicsMovement _selfcreature))
  (bind _creaturebehaviorsettings (Utilities|Struct|BreakS_CreatureDetailsInstanced _userdata))
  (bind (_rotationratedegs _speedms) (Utilities|Struct|BreakS_AICreatureBehaviorSettings _creaturebehaviorsettings))
  (Variables|/Game/Blueprints/AddOn/Components/BPC_ActorPhysicsMovement.BPC_ActorPhysicsMovement_C|SetRotationRate _bpc_actorphysicsmovement (.Neutre (Utilities|Struct|BreakS_FloatCreatureMode _rotationratedegs)))
  (Variables|/Game/Blueprints/AddOn/Components/BPC_ActorPhysicsMovement.BPC_ActorPhysicsMovement_C|SetTargetSpeed _bpc_actorphysicsmovement (.Neutre (Utilities|Struct|BreakS_FloatCreatureMode _speedms)))
  (return))