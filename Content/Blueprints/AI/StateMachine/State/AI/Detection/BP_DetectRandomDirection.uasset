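; BP_DetectRandomDirection is an AI detection state that gives its creature a random movement direction.
; On update, it calls SetRandomDirection on the creature's physics movement component with a fixed cone angle and coverage, using the forward detection distance from the AI data as range.
; It then runs the parent update and immediately requests a detection state change, while start and quit only defer to the parent.
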(event EventIStart
  (|CallParentFunction))

(event EventIUpdate
  (params (DeltaSeconds :type Float%20%28double-precision%29))
  (bind _selfcreature (Variables|Default|GetSelfCreature))
  (Default|SetRandomDirection (Variables|/Game/Blueprints/AI/Pawn/BP_CreatureGeneric.BP_CreatureGeneric_C|GetBPC_ActorPhysicsMovement _selfcreature) 3e+01 (Utilities|Struct|BreakS_AICreatureBehaviorSettings (Default|GetAIData _selfcreature)) 180)
  (|CallParentFunction DeltaSeconds)
  (CallFunction|IChangeState (Utilities|Enum|LiteralenumE_StateDetection "NewEnumerator0")))

(event EventIQuit
  (|CallParentFunction))