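; BP_DetectSpline is an AI detection state in a state machine that steers a creature along its current spline.
; On init it caches the target's BPC_FollowSpline component.
; Each update it feeds the spline direction, computed from the creature's location and a look-ahead point along its forward vector, into BPCActorPhysicsMovement.
; It then requests a detection state change every update, with no condition.
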(event EventIStart
  (|CallParentFunction))

(event EventIUpdate
  (params (DeltaSeconds :type Float%20%28double-precision%29))
  (bind _selfcreature (Variables|Default|GetSelfCreature))
  (bind _returnvalue (Transformation|GetActorLocation _selfcreature))
  (Default|AddDirection (Variables|/Game/Blueprints/AI/Pawn/BP_CreatureGeneric.BP_CreatureGeneric_C|GetBPC_ActorPhysicsMovement (Variables|Default|GetSelfCreature)) (Default|GetDirectiontoNearestPoint (Default|GetCurrentSpline (Variables|Default|GetBPC_FollowSpline)) _returnvalue (+ _returnvalue (* (Transformation|GetActorForwardVector _selfcreature) 1.5e+03))))
  (|CallParentFunction DeltaSeconds)
  (CallFunction|IChangeState (Utilities|Enum|LiteralenumE_StateDetection "NewEnumerator0")))

(event EventIQuit
  (|CallParentFunction))

(fn InitState
  (params (Target :type Actor%20Object%20Reference) (StateName :type Byte :default 0) (Commander :type BP%20State%20Commander%20Object%20Reference))
  (|CallParentFunction Target StateName Commander)
  (bind _asbpc_follow_spline (Utilities|Casting|CastToBPC_FollowSpline (CallFunction|TryGetComponent (Variables|Default|GetTarget) "/Game/Blueprints/AddOn/Components/GenericComponents/BPC_FollowSpline.BPC_FollowSpline_C")))
  (Variables|Default|SetBPC_FollowSpline _asbpc_follow_spline))