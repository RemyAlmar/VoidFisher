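; BP_DetectObstacle is an AI detection state that steers a creature toward free space while its path is blocked.
; Each update, it asks the creature's physics movement component whether the current direction is clear, using an extended forward detection distance from the AI data.
; If clear, it switches to another detection state; otherwise, it sets a free direction within a cone around the actor's forward vector.
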(event EventIStart
  (|CallParentFunction))

(event EventIUpdate
  (params (DeltaSeconds :type Float%20%28double-precision%29))
  (bind _selfcreature (Variables|Default|GetSelfCreature))
  (bind _selfcreature_2 (Variables|Default|GetSelfCreature))
  (if (Default|CanMovetoCurrentDirection (Variables|/Game/Blueprints/AI/Pawn/BP_CreatureGeneric.BP_CreatureGeneric_C|GetBPC_ActorPhysicsMovement _selfcreature_2) (* (Utilities|Struct|BreakS_AICreatureBehaviorSettings (Default|GetAIData _selfcreature_2)) 1.5))
    (CallFunction|IChangeState (Utilities|Enum|LiteralenumE_StateDetection "NewEnumerator0"))
    (else
      (Default|SetFreeDirectiontoMove _selfcreature 6e+01 (Transformation|GetActorForwardVector _selfcreature))))
  (|CallParentFunction DeltaSeconds))

(event EventIQuit
  (|CallParentFunction))