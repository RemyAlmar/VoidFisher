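; AI behavior state that makes a creature dodge in a random zigzag direction when it uses its skill.
; UseSkill randomly picks left or right, rotates the forward vector 90–180 degrees around up, and adds that scaled direction to physics movement before calling the parent.
; InitState creates a sphere on the creature, sized from its detection radius and the Commander's normalized distance for this state.
; Updates defer to the parent state.
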(event EventIUpdate
  (params (DeltaSeconds :type Float%20%28double-precision%29))
  (|CallParentFunction DeltaSeconds))

(fn GetDirectioninConeDynamic
  (params (TargetDirection :type Vector) (UpVector :type Vector) (InputDirection :type Vector%202D%20Structure) (Angle :type Float%20%28double-precision%29))
  (LocalVariables|SetRightVector (Math|Vector|Normalize (Math|Vector|CrossProduct UpVector TargetDirection)))
  (LocalVariables|SetEdgeDirection (Math|Vector|RotateVectorAroundAxis TargetDirection (* Angle (.y InputDirection)) (LocalVariables|GetRightVector)))
  (LocalVariables|SetFinalDirection (Math|Vector|RotateVectorAroundAxis (LocalVariables|GetEdgeDirection) (* (.x InputDirection) Angle) UpVector))
  (return (LocalVariables|GetFinalDirection)))

(fn UseSkill
  (bind _selfcreature (Variables|Default|GetSelfCreature))
  (if (Math|Random|RandomBoolwithWeight 0.5)
    (LocalVariables|SetXDirection (Math|Random|RandomFloatinRange 0.5 1.0))
    (else
      (LocalVariables|SetXDirection (Math|Random|RandomFloatinRange -1.0 -0.5))))
  (bind _output_get (CallFunction|GetDirectioninConeDynamic (Transformation|GetActorForwardVector _selfcreature) (Transformation|GetActorUpVector _selfcreature) (Math|Vector2D|MakeVector2D (LocalVariables|GetXDirection) 0.0) 1.8e+02))
  (Default|AddDirection (Variables|/Game/Blueprints/AI/Pawn/BP_CreatureGeneric.BP_CreatureGeneric_C|GetBPC_ActorPhysicsMovement (Variables|Default|GetSelfCreature)) (* _output_get 3e+01))
  (|CallParentFunction))

(fn InitState
  (params (Target :type Actor%20Object%20Reference) (StateName :type Byte :default 0) (Commander :type BP%20State%20Commander%20Object%20Reference))
  (bind _selfcreature (Variables|Default|GetSelfCreature))
  (|CallParentFunction Target StateName Commander)
  (Default|CreateSphere _selfcreature (* (Variables|/Script/Engine.SphereComponent|GetSphereRadius (Variables|/Game/Blueprints/AI/Pawn/BP_CreatureGeneric.BP_CreatureGeneric_C|GetDetectionArea _selfcreature)) (.Value (Utilities|Map|Find (Variables|/Game/Blueprints/AI/StateMachine/BP_StateCommander.BP_StateCommander_C|GetListDistanceNormalized Commander) StateName))) false))