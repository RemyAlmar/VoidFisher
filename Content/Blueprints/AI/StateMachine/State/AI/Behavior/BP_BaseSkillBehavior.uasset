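; Base AI state machine behavior for creature skills, extending a parent cooldown behavior with availability and usability gating.
; Each update either fires the skill when available and usable, or advances the cooldown timer, whose reset makes it available again; zero cooldown keeps it available.
; Setters raise events only on value changes, and UseSkill just clears CanUseSkill.
; Skill range is the creature's detection sphere radius scaled by a normalized distance.
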(event Custom|OnCanUseValueChanged_Event
  (params (CanUseSkill :type Boolean)))

(event Custom|OnSkillAvailableValueChanged_Event
  (params (SkillAvailable :type Boolean)))

(event Custom|WhileSkillAvailable_Event
  (params (DeltaTime :type Float%20%28double-precision%29))
  (if (Variables|Default|GetCanUseSkill)
    (CallFunction|UseSkill)
    (CallFunction|SetSkillAvailable (<= (Variables|Default|GetCooldownMax) 0.0)) ; Pour garder le skill disponible si on a mis le cooldown à 0
  ))

(event EventIUpdate
  (params (DeltaSeconds :type Float%20%28double-precision%29))
  (if (Variables|Default|GetSkill%20Available)
    (CallFunction|WhileSkillAvailableEvent DeltaSeconds)
    (elif (CallFunction|TimerPos (Variables|Default|GetCurrentTime) DeltaSeconds (Variables|Default|GetCooldownMax) true)
      (CallFunction|EDonCooldownResetEvent)
      (else
        (CallFunction|SetStartCooldown true)
        (CallFunction|EDonCooldownUpdateEvent DeltaSeconds)))))

(event EventEDonCooldownResetEvent
  (|CallParentFunction)
  (CallFunction|SetSkillAvailable true))

(fn GetRangeDistance
  (return (* (Variables|/Script/Engine.SphereComponent|GetSphereRadius (Variables|/Game/Blueprints/AI/Pawn/BP_CreatureGeneric.BP_CreatureGeneric_C|GetDetectionArea (Variables|Default|GetSelfCreature))) (CallFunction|GetDistanceNormalized))))

(fn SetSkillAvailable
  (params (Skill%20Available :type Boolean))
  (LocalVariables|SetPreviousValue (Variables|Default|GetSkill%20Available))
  (Variables|Default|SetSkill%20Available Skill%20Available)
  (if (!= (Variables|Default|GetSkill%20Available) (LocalVariables|GetPreviousValue))
    (CallFunction|OnSkillAvailableValueChangedEvent (Variables|Default|GetSkill%20Available))))

(fn SetCanUseSkill
  (params (CanUseSkill :type Boolean))
  (LocalVariables|SetPreviousValue (Variables|Default|GetCanUseSkill))
  (Variables|Default|SetCanUseSkill CanUseSkill)
  (if (!= (Variables|Default|GetCanUseSkill) (LocalVariables|GetPreviousValue))
    (CallFunction|OnCanUseValueChangedEvent (Variables|Default|GetCanUseSkill))))

(fn UseSkill
  (CallFunction|SetCanUseSkill false))