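; BP_NeutralBehavior is the neutral behavior state in the AI state machine, where the AI waits out a cooldown before switching to a skill state.
; Entering resets the timer to its maximum, which SetCooldownTime can configure.
; Each update counts it down with clamping, then requests the state change on the update after it reaches zero.
; Parent state logic still runs, and debug text shows the state and remaining time.
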(event EventIStart
  (Variables|Cooldown|SetCurrentTime (Variables|Cooldown|GetMaxCooldown))
  (Variables|Default|SetSkill%20Available false)
  (|CallParentFunction))

(event EventIUpdate
  (params (DeltaSeconds :type Float%20%28double-precision%29))
  (Development|PrintText 0 "NEUTRAL" true true "(R=1.000000,G=0.316460,B=0.000000,A=1.000000)" 0.0)
  (if (Variables|Default|GetSkill%20Available)
    (CallFunction|IChangeState (Utilities|Enum|LiteralenumE_StateSkills "NewEnumerator0"))
    (else
      (CallFunction|ResetCooldown DeltaSeconds)))
  (|CallParentFunction DeltaSeconds))

(event EventIQuit
  (|CallParentFunction))

(fn ResetCooldown
  (params (DeltaTime :type Float%20%28double-precision%29))
  (Variables|Cooldown|SetCurrentTime (Math|Float|Clamp(Float) (- (Variables|Cooldown|GetCurrentTime) DeltaTime) 0.0 (Variables|Cooldown|GetMaxCooldown)))
  (Variables|Default|SetSkill%20Available (<= (Variables|Cooldown|GetCurrentTime) 0.0))
  (Development|PrintText 0 (Utilities|Text|FormatText "Temps Restant : {x}s/ {y}s" (Variables|Cooldown|GetCurrentTime) (Variables|Cooldown|GetMaxCooldown)) true true "(R=1.000000,G=0.953193,B=0.104348,A=1.000000)" 0.0))

(fn SetCooldownTime
  (params (MaxCooldown :type Float%20%28double-precision%29))
  (bind _output_get (Variables|Cooldown|SetMaxCooldown MaxCooldown))
  (Variables|Cooldown|SetCurrentTime _output_get))