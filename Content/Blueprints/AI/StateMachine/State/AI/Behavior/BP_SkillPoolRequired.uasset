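; Base AI state machine behavior for skills that need an actor pool on their creature.
; On init, it runs the parent setup and caches the creature's BPC_ParamsByString component.
; It then reuses the creature's BPC_PoolActorSpawner whose spawn class matches ActorPoolClass, or adds a new one if none exists, so pools are looked up per actor class.
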(fn InitState
  (params (Target :type Actor%20Object%20Reference) (StateName :type Byte :default 0) (Commander :type BP%20State%20Commander%20Object%20Reference))
  (|CallParentFunction Target StateName Commander)
  (bind _asbpc_params_by_string (Utilities|Casting|CastToBPC_ParamsByString (CallFunction|TryGetComponent (Variables|Default|GetSelfCreature) "/Game/Blueprints/AddOn/Components/GenericComponents/BPC_ParamsByString.BPC_ParamsByString_C"))
    (:then
      (Variables|Default|SetBPC_Params _asbpc_params_by_string))
    (:CastFailed
      _))
  ;[0 1 0.4217] Recuperation / Creation / Initialisation du Pool
  (bind _output_get (Variables|Default|SetBPCPool (PoolHandling|GetPoolRequired (Actor|GetComponentsByClass (Variables|Default|GetSelfCreature) "/Game/Blueprints/AddOn/Components/BPC_PoolActorSpawner.BPC_PoolActorSpawner_C") (Variables|Default|GetActorPoolClass))))
  (Utilities|IsValid _output_get
    (:Is%20Not%20Valid
      (bind _returnvalue (Game|AddComponentbyClass (Variables|Default|GetSelfCreature) "/Game/Blueprints/AddOn/Components/BPC_PoolActorSpawner.BPC_PoolActorSpawner_C" (Variables|Default|GetActorPoolClass)))
      (Variables|Default|SetBPCPool _returnvalue))))

(fn GetPoolRequired
  (params (Array :type Array%20of%20BPC%20Pool%20Actor%20Spawner%20Object%20References) (PoolActorClass :type Object%20Class%20Reference))
  (for _array_element Array
    (if (== (Variables|/Game/Blueprints/AddOn/Components/BPC_PoolActorSpawner.BPC_PoolActorSpawner_C|GetClass%20to%20Spawn _array_element) PoolActorClass)
      (LocalVariables|SetPool _array_element)
      (return (LocalVariables|GetPool))))
  (return (LocalVariables|GetPool)))