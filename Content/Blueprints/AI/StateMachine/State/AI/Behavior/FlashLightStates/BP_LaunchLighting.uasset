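; AI creature state for the launch step of a flash attack, which flashbangs players the creature is seen by or seeing via its prey component.
; On start it adds the flashbang widget to those actors' screens, fires the skill-use event and spawns a Niagara flash on the mesh socket.
; During the cooldown it animates a dynamic material mask and eases mesh rotation to zero, then switches to state 3.
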(event EventEDonCooldownResetEvent
  (Default|IChangeState (Variables|Default|GetCommander) 3))

(event EventIQuit
  (Default|SetScalarParameter (Variables|Default|GetBPC_DynamicalMaterialManager) (Variables|Default|GetMaterialName) 0 "Mask" -1.0)
  (|CallParentFunction))

(event EventEDonCooldownUpdateEvent
  (params (DeltaTime :type Float%20%28double-precision%29))
  (Default|SetScalarParameter (Variables|Default|GetBPC_DynamicalMaterialManager) (Variables|Default|GetMaterialName) 0 "Mask" (Math|Float|Lerp -1.0 1.0 (CallFunction|GetInverseTimeNormalized)))
  (Transformation|SetRelativeRotation (Variables|/Game/Blueprints/AI/Pawn/BP_CreatureGeneric.BP_CreatureGeneric_C|GetSKM_Creature (Variables|Default|GetSelfCreature)) (Math|Rotator|Lerp(Rotator) (Variables|Default|GetTargetRotation) "0, 0, 0" (CallFunction|GetNormalizedTime) true) false false)
  (|CallParentFunction DeltaTime))

(event EventIStart
  (bind _selfcreature (Variables|Default|GetSelfCreature))
  (for _array_element (Variables|/Game/Blueprints/AddOn/Components/BPC_Prey.BPC_Prey_C|GetActorSeeing (Variables|/Game/Blueprints/AI/Pawn/BP_CreatureGeneric.BP_CreatureGeneric_C|GetBPC_Prey (Variables|Default|GetSelfCreature)))
    (Utilities|IsValid (Actor|GetComponentbyClass _array_element "/Game/Blueprints/AddOn/Components/BPC_WidgetManager.BPC_WidgetManager_C")
      (:Is%20Valid
        (Default|AddWidgettoPlayerScreen (Actor|GetComponentbyClass _array_element "/Game/Blueprints/AddOn/Components/BPC_WidgetManager.BPC_WidgetManager_C") "/Game/Blueprints/Widgets/Misc/UI_Flashbang.UI_Flashbang_C" true))))
  (|CallParentFunction)
  (Default|CallEDonUseSkill _selfcreature)
  (Variables|Default|SetTargetRotation (Variables|/Script/Engine.SceneComponent|GetRelativeRotation (Variables|/Game/Blueprints/AI/Pawn/BP_CreatureGeneric.BP_CreatureGeneric_C|GetSKM_Creature (Variables|Default|GetSelfCreature))))
  (Niagara|SpawnSystemAttached "/Game/VFX/Niagara/Fish/NS_Flash.NS_Flash" (Variables|/Game/Blueprints/AI/Pawn/BP_CreatureGeneric.BP_CreatureGeneric_C|GetSKM_Creature _selfcreature) "VFX_Socket_Flash" "0.000000,0.000000,0.000000" "0, 0, 0" "SnapToTarget" true))

(fn InitState
  (params (Target :type Actor%20Object%20Reference) (StateName :type Byte :default 0) (Commander :type BP%20State%20Commander%20Object%20Reference))
  (|CallParentFunction Target StateName Commander)
  (bind _asbpc_dynamical_material_manager (Utilities|Casting|CastToBPC_DynamicalMaterialManager (CallFunction|GetComponentInstance (Variables|Default|GetSelfCreature) "/Game/Blueprints/AddOn/Components/BPC_DynamicalMaterialManager.BPC_DynamicalMaterialManager_C")))
  (bind _output_get (Variables|Default|SetBPC_DynamicalMaterialManager _asbpc_dynamical_material_manager))
  (Default|AddNewMaterialInstanceDynamical _output_get "/Game/Asset/Materials/FISH/Medium/MI_Shineon.MI_Shineon" (Variables|Default|GetMaterialName)))