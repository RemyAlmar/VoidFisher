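; Flashlight AI behavior state that loads a creature's lighting skill over a cooldown, shown through a dynamic shine material.
; Cooldown updates drive the material's Mask scalar, and start and quit resync the timer from that value to continue from another state's progress.
; Cooldown reset switches the commander to state 1.
; Prey predator-reaction events disable the skill while a predator is present and re-enable it afterwards.
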(event EventEDonCooldownResetEvent
  (Default|IChangeState (Variables|Default|GetCommander) 1)
  (|CallParentFunction))

(event EventEDonCooldownUpdateEvent
  (Default|SetScalarParameter (Variables|Default|GetBPC_DynamicalMaterialManager) (Variables|Default|GetMaterialName) 0 "Mask" (Math|Float|Lerp -1.0 1.0 (CallFunction|GetNormalizedTime)))
  (|CallParentFunction))

(event EventIStart
  (CallFunction|SetCurrentTimebyNormalizedValue (Math|Float|NormalizetoRange (Default|GetScalarParameterValue (Variables|Default|GetBPC_DynamicalMaterialManager) "Mask") -1.0 1.0)) ; Met le current time par rapport à la valeur de celui de l'autre etat
  (Default|SetScalarParameter (Variables|Default|GetBPC_DynamicalMaterialManager) (Variables|Default|GetMaterialName) 0 "Mask" (Math|Float|Lerp -1.0 1.0 (CallFunction|GetNormalizedTime)))
  (Default|CallEDonLoadSkill (Variables|Default|GetSelfCreature))
  (|CallParentFunction))

(event EventIQuit
  (CallFunction|SetCurrentTimebyNormalizedValue (Math|Float|NormalizetoRange (Default|GetScalarParameterValue (Variables|Default|GetBPC_DynamicalMaterialManager) "Mask") -1.0 1.0))
  (|CallParentFunction))

(event EventBPCPreyEDReactonPredatorin
  (params (TargetPredator :type Actor%20Object%20Reference))
  ;[0.1998 1 0.09453] Active / Desactive l'update (True = desactive / Faux = Active)
  (CallFunction|SetSkillAvailable false))

(event EventBPCPreyEDonWithoutPredatorEvent
  ;[0.1998 1 0.09453] Active / Desactive l'update (True = desactive / Faux = Active)
  (CallFunction|SetSkillAvailable true))

(fn InitState
  (params (Target :type Actor%20Object%20Reference) (StateName :type Byte :default 0) (Commander :type BP%20State%20Commander%20Object%20Reference))
  (|CallParentFunction Target StateName Commander)
  (bind _asbpc_dynamical_material_manager (Utilities|Casting|CastToBPC_DynamicalMaterialManager (CallFunction|GetComponentInstance (Variables|Default|GetSelfCreature) "/Game/Blueprints/AddOn/Components/BPC_DynamicalMaterialManager.BPC_DynamicalMaterialManager_C")))
  (Variables|Default|SetBPC_DynamicalMaterialManager _asbpc_dynamical_material_manager)
  (Default|AddNewMaterialInstanceDynamical (Variables|Default|GetBPC_DynamicalMaterialManager) "/Game/Asset/Materials/FISH/Medium/MI_Shineon.MI_Shineon" (Variables|Default|GetMaterialName))
  (Default|AddScalarParameter (Variables|Default|GetBPC_DynamicalMaterialManager) "Mask" -1.0))