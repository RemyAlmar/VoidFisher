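; AI state machine state for a creature's flashlight behavior, covering the reload of its lighting skill.
; On init it finds the creature's dynamic material manager component and registers a dynamic instance of the shine material.
; On start it fires the creature's reload-skill dispatcher, and when the cooldown reset event arrives it tells the Commander to switch to state 0.
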(event EventEDonCooldownResetEvent
  (Default|IChangeState (Variables|Default|GetCommander)))

(event EventIStart
  (|CallParentFunction)
  (Default|CallEDonReloadSkill (Variables|Default|GetSelfCreature)))

(fn InitState
  (params (Target :type Actor%20Object%20Reference) (StateName :type Byte :default 0) (Commander :type BP%20State%20Commander%20Object%20Reference))
  (|CallParentFunction Target StateName Commander)
  (bind _asbpc_dynamical_material_manager (Utilities|Casting|CastToBPC_DynamicalMaterialManager (CallFunction|GetComponentInstance (Variables|Default|GetSelfCreature) "/Game/Blueprints/AddOn/Components/BPC_DynamicalMaterialManager.BPC_DynamicalMaterialManager_C")))
  (bind _output_get (Variables|Default|SetBPC_DynamicalMaterialManager _asbpc_dynamical_material_manager))
  (Default|AddNewMaterialInstanceDynamical _output_get "/Game/Asset/Materials/FISH/Medium/MI_Shineon.MI_Shineon" (Variables|Default|GetMaterialName)))