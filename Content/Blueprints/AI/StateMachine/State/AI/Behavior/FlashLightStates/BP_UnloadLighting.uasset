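; AI behavior state that unloads a creature's flashlight glow, driving the "Mask" scalar of a dynamic Shineon material through BPC_DynamicalMaterialManager.
; Each cooldown update lerps Mask between -1 and 1 by inverse normalized time.
; On start and quit, it derives cooldown time from the current Mask value to resume partial fades.
; It switches to state 0 when the cooldown resets or BPCPrey detects no predator within range.
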(event EventEDonCooldownResetEvent
  (Default|IChangeState (Variables|Default|GetCommander))
  (|CallParentFunction))

(event EventIQuit
  (CallFunction|SetCurrentTimebyNormalizedValue (Math|Float|NormalizetoRange (Default|GetScalarParameterValue (Variables|Default|GetBPC_DynamicalMaterialManager) "Mask") -1.0 1.0))
  (Development|PrintText 0 "Quit Unload " true true "(R=1.000000,G=0.000000,B=0.607821,A=1.000000)" 3.0)
  (|CallParentFunction))

(event EventEDonCooldownUpdateEvent
  (Default|SetScalarParameter (Variables|Default|GetBPC_DynamicalMaterialManager) (Variables|Default|GetMaterialName) 0 "Mask" (Math|Float|Lerp -1.0 1.0 (CallFunction|GetInverseTimeNormalized)))
  (Development|PrintText 0 "Unload " true true "(R=1.000000,G=0.385595,B=0.000000,A=1.000000)" 0.0)
  (if (Default|HasPredatorNear (Variables|/Game/Blueprints/AI/Pawn/BP_CreatureGeneric.BP_CreatureGeneric_C|GetBPC_Prey (Variables|Default|GetSelfCreature)) (CallFunction|GetRangeDistance))
    _
    (else
      (Default|IChangeState (Variables|Default|GetCommander)) ; Va Charger quand Predator proche
    ))
  (|CallParentFunction))

(event EventIStart
  (CallFunction|SetCurrentTimebyNormalizedValue (Math|Float|NormalizetoRange (Default|GetScalarParameterValue (Variables|Default|GetBPC_DynamicalMaterialManager) "Mask") -1.0 1.0)) ; Met le current time par rapport à la valeur de celui de l'autre etat
  (Default|SetScalarParameter (Variables|Default|GetBPC_DynamicalMaterialManager) (Variables|Default|GetMaterialName) 0 "Mask" (Math|Float|Lerp -1.0 1.0 (CallFunction|GetInverseTimeNormalized)))
  (Development|PrintText 0 "Start Unload " true true "(R=0.000000,G=1.000000,B=0.948432,A=1.000000)" 3.0)
  (|CallParentFunction))

(fn InitState
  (params (Target :type Actor%20Object%20Reference) (StateName :type Byte :default 0) (Commander :type BP%20State%20Commander%20Object%20Reference))
  (|CallParentFunction Target StateName Commander)
  (bind _asbpc_dynamical_material_manager (Utilities|Casting|CastToBPC_DynamicalMaterialManager (CallFunction|GetComponentInstance (Variables|Default|GetSelfCreature) "/Game/Blueprints/AddOn/Components/BPC_DynamicalMaterialManager.BPC_DynamicalMaterialManager_C")))
  (bind _output_get (Variables|Default|SetBPC_DynamicalMaterialManager _asbpc_dynamical_material_manager))
  (Default|AddNewMaterialInstanceDynamical _output_get "/Game/Asset/Materials/FISH/Medium/MI_Shineon.MI_Shineon" (Variables|Default|GetMaterialName))
  (Default|CreateSphere (Variables|Default|GetSelfCreature) (CallFunction|GetRangeDistance)))