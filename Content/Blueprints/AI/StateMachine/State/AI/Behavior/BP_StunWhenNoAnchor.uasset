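; An AI behavior state that stuns the creature once it has no active anchors left.
; InitState finds the creature's BPC_AnchorManager and binds to its hook-detach event.
; On each detach it checks for active anchors and, when none remain, adds and immediately starts BP_Stunned on the creature's movement state manager.
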(event Custom|OnAllAnchorDeactivate
  (if (not (Default|HasAnchorActive (Variables|Default|GetBPCAnchorManager)))
    (Default|AddState (Variables|/Game/Blueprints/AI/Pawn/BP_CreatureGeneric.BP_CreatureGeneric_C|GetBPC_StateManager_Movement (Variables|Default|GetSelfCreature)) (Utilities|Enum|LiteralenumE_StateMovement "NewEnumerator3") true "/Game/Blueprints/AI/StateMachine/State/AI/Movement/BP_Stunned.BP_Stunned_C")))

(event Custom|BPC_Anchor_ED_OnDetachHook_Event
  (if (not (Default|HasAnchorActive (Variables|Default|GetBPCAnchorManager)))
    (CallFunction|OnAllAnchorDeactivate)))

(fn InitState
  (params (Target :type Actor%20Object%20Reference) (StateName :type Byte :default 0) (Commander :type BP%20State%20Commander%20Object%20Reference))
  (|CallParentFunction Target StateName Commander)
  (bind _asbpc_anchor_manager (Utilities|Casting|CastToBPC_AnchorManager (CallFunction|TryGetComponent (Variables|Default|GetSelfCreature) "/Game/Blueprints/AddOn/Components/BPC_AnchorManager.BPC_AnchorManager_C")))
  (bind _output_get (Variables|Default|SetBPCAnchorManager _asbpc_anchor_manager))
  (EventDispatchers|BindEventtoEDonDetachHook _output_get (EventDispatchers|CreateEvent :!event Custom|BPC_Anchor_ED_OnDetachHook_Event)))