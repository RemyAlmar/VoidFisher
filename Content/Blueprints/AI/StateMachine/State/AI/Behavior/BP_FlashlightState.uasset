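; BP_FlashlightState is an AI behavior state for a creature, running its own nested state machine of sub-states.
; On init it scales each sub-state's normalized distance by its own and sets the last one's cooldown to CooldownMax.
; It then constructs a child StateCommander from that list and creates a hidden sphere on the creature, sized from its detection radius and the state's normalized distance.
; Each update is forwarded to the child commander.
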(event EventIUpdate
  (params (DeltaSeconds :type Float%20%28double-precision%29))
  (Default|IUpdate (Variables|Default|GetStateCommander) DeltaSeconds))

(fn InitState
  (params (Target :type Actor%20Object%20Reference) (StateName :type Byte :default 0) (Commander :type BP%20State%20Commander%20Object%20Reference))
  (bind _selfcreature (Variables|Default|GetSelfCreature))
  (|CallParentFunction Target StateName Commander)
  (CallFunction|SetParamtoStates)
  (bind _returnvalue (Game|ConstructObjectfromClass "/Game/Blueprints/AI/StateMachine/BP_StateCommander.BP_StateCommander_C"))
  (bind _output_get (Variables|Default|SetStateCommander _returnvalue))
  (Default|InititalizeCommander _output_get _selfcreature (Variables|Default|GetList%20States%20Class))
  (Default|CreateSphere _selfcreature (* (Variables|/Script/Engine.SphereComponent|GetSphereRadius (Variables|/Game/Blueprints/AI/Pawn/BP_CreatureGeneric.BP_CreatureGeneric_C|GetDetectionArea _selfcreature)) (CallFunction|GetDistanceNormalized)) true))

(fn SetParamtoStates
  (bind _values (Utilities|Map|Values (Variables|Default|GetList%20States%20Class)))
  (for (_array_element _array_index) _values
    (LocalVariables|SetCurrentIndex _array_index)
    (LocalVariables|SetCooldown (.Cooldown (Utilities|Struct|BreakS_StateCooldown _array_element)))
    (if (== (LocalVariables|GetCurrentIndex) (Utilities|Array|LastIndex _values))
      (LocalVariables|SetCooldown (Variables|Default|GetCooldownMax)))
    (LocalVariables|SetNextValue (Utilities|Struct|MakeS_StateCooldown (.State (Utilities|Struct|BreakS_StateCooldown _array_element)) (LocalVariables|GetCooldown) (* (CallFunction|GetDistanceNormalized) (.DistanceNormalized (Utilities|Struct|BreakS_StateCooldown _array_element)))))
    (bind _keys (Utilities|Map|Keys (Variables|Default|GetList%20States%20Class)))
    (Utilities|Map|Add (LocalVariables|GetNextMap) (Utilities|Array|Get(acopy) _keys (LocalVariables|GetCurrentIndex)) (LocalVariables|GetNextValue)))
  (|SetBy-RefVar (Variables|Default|GetList%20States%20Class) (LocalVariables|GetNextMap))
  (return))