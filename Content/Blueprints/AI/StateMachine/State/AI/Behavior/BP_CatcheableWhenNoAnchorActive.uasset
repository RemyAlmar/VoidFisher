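; AI behavior state that ties a creature's catchable status to its anchors, allowing capture only when none are active.
; InitState fetches the creature's BPC_AnchorManager and binds to its anchor event dispatcher.
; An overlap-change handler sets catchability to the inverse of HasAnchorActive.
; An all-anchors-deactivated handler switches a Niagara material parameter to the net material through the creature's VFX manager.
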(event Custom|BPCAnchor_ED_OnAllAnchorDeactivate_Event
  (Default|SetMaterialNiagaraSystem (Variables|/Game/Blueprints/AI/Pawn/BP_CreatureGeneric.BP_CreatureGeneric_C|GetBPC_VFX_Manager (Variables|Default|GetSelfCreature)) "NewEnumerator1" "Material" "/Game/VFX/Materials/Fish/M_Net.M_Net"))

(event Custom|BPCAnchor_ED_OnChangeAllOverlap_Event
  (Default|SetIsCatcheable (Variables|Default|GetSelfCreature) (not (Default|HasAnchorActive (Variables|Default|GetBPC_AnchorManager)))))

(fn InitState
  (params (Target :type Actor%20Object%20Reference) (StateName :type Byte :default 0) (Commander :type BP%20State%20Commander%20Object%20Reference))
  (|CallParentFunction Target StateName Commander)
  (bind _asbpc_anchor_manager (Utilities|Casting|CastToBPC_AnchorManager (CallFunction|TryGetComponent (Variables|Default|GetSelfCreature) "/Game/Blueprints/AddOn/Components/BPC_AnchorManager.BPC_AnchorManager_C")))
  (bind _output_get (Variables|Default|SetBPC_AnchorManager _asbpc_anchor_manager))
  (EventDispatchers|BindEventtoEDonAllAnchorDeactivate _output_get (EventDispatchers|CreateEvent :!event Custom|BPCAnchor_ED_OnAllAnchorDeactivate_Event)))