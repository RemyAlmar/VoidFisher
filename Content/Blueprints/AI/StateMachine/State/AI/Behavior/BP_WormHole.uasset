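; AI skill state that gives a creature a random zig-zag direction change when it starts.
; On start it picks left or right at even odds and rotates the creature's forward vector around its up axis by a random 90 to 180 degrees.
; The result is stored in the creature's DirectionAdditive, and the first update requests a switch to another skill state, with debug prints along the way.
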(event EventIStart
  (CallFunction|UseSkill)
  (|CallParentFunction))

(event EventIUpdate
  (params (DeltaSeconds :type Float%20%28double-precision%29))
  (Development|PrintText 0 "WormHole" true true "(R=0.000000,G=1.000000,B=0.485315,A=1.000000)" 0.0)
  (CallFunction|IChangeState (Utilities|Enum|LiteralenumE_StateSkills "NewEnumerator3"))
  (|CallParentFunction DeltaSeconds))

(event EventIQuit
  (|CallParentFunction))

(event EventIChangeState
  (params (TargetState :type Byte :default 0))
  (|CallParentFunction TargetState))

(fn UseSkill
  (bind _selfcreature (Variables|Default|GetSelfCreature))
  (if (Math|Random|RandomBoolwithWeight 0.5)
    (LocalVariables|SetXDirection (Math|Random|RandomFloatinRange 0.5 1.0))
    (Development|PrintText 0 "ZIG" true true "(R=1.000000,G=0.509934,B=0.000000,A=1.000000)" 3.0)
    (else
      (LocalVariables|SetXDirection (Math|Random|RandomFloatinRange -1.0 -0.5))
      (Development|PrintText 0 "ZAG" true true "(R=1.000000,G=0.509934,B=0.000000,A=1.000000)" 3.0)))
  (bind _output_get (CallFunction|GetDirectioninConeDynamic (Transformation|GetActorForwardVector _selfcreature) (Transformation|GetActorUpVector _selfcreature) (Math|Vector2D|MakeVector2D (LocalVariables|GetXDirection) 0.0) 1.8e+02))
  (bind _output_get_2 (Variables|/Game/Blueprints/AI/Pawn/BP_Fish.BP_Fish_C|SetDirectionAdditive (Variables|Default|GetSelfCreature) _output_get))
  (Development|PrintText 0 (Utilities|Text|FormatText "Add Direction ZIG ZAG : {x}" (Utilities|String|ToString(Vector) _output_get_2)) true true "(R=1.000000,G=0.365145,B=0.000000,A=1.000000)")
  (return))

(fn GetDirectioninConeDynamic
  (params (TargetDirection :type Vector) (UpVector :type Vector) (InputDirection :type Vector%202D%20Structure) (Angle :type Float%20%28double-precision%29))
  (LocalVariables|SetRightVector (Math|Vector|Normalize (Math|Vector|CrossProduct UpVector TargetDirection)))
  (LocalVariables|SetEdgeDirection (Math|Vector|RotateVectorAroundAxis TargetDirection (* Angle (.y InputDirection)) (LocalVariables|GetRightVector)))
  (LocalVariables|SetFinalDirection (Math|Vector|RotateVectorAroundAxis (LocalVariables|GetEdgeDirection) (* (.x InputDirection) Angle) UpVector))
  (return (LocalVariables|GetFinalDirection)))