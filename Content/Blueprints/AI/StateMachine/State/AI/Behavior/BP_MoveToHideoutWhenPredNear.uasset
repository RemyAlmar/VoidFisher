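; AI behavior skill state that steers prey creatures toward the nearest known hideout when a predator is near.
; InitState reuses or adds a BPC_GetHideout component, initialized with the creature's detection area.
; Predator events toggle the skill, whose use pushes movement direction toward the hideout and prints the target.
; Reaching the hideout starts BP_Idle in the movement state manager, while losing the predator starts BP_MoveAI.
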(event Custom|ED_OnHideoutLeaved_Event)

(event Custom|ED_OnHideoutReached_Event
  (Default|AddState (Variables|/Game/Blueprints/AI/Pawn/BP_CreatureGeneric.BP_CreatureGeneric_C|GetBPC_StateManager_Movement (Variables|Default|GetSelfCreature)) (Utilities|Enum|LiteralenumE_StateMovement "NewEnumerator0") true "/Game/Blueprints/AI/StateMachine/State/AI/Movement/BP_Idle.BP_Idle_C"))

(event EventBPCPreyEDSeePredatorinRange
  (params (TargetPredator :type Actor%20Object%20Reference))
  (CallFunction|SetCanUseSkill (and (Default|HasHideoutKnown (Variables|Default|GetBPC_GetHideout)) (Default|HasPredatorNear (Variables|/Game/Blueprints/AI/Pawn/BP_CreatureGeneric.BP_CreatureGeneric_C|GetBPC_Prey (Variables|Default|GetSelfCreature)) (CallFunction|GetRangeDistance)))))

(event EventBPCPreyEDWithoutPredatorEvent
  (CallFunction|SetCanUseSkill false)
  (Default|AddState (Variables|/Game/Blueprints/AI/Pawn/BP_CreatureGeneric.BP_CreatureGeneric_C|GetBPC_StateManager_Movement (Variables|Default|GetSelfCreature)) (Utilities|Enum|LiteralenumE_StateMovement "NewEnumerator1") true "/Game/Blueprints/AI/StateMachine/State/AI/Movement/BP_MoveAI.BP_MoveAI_C"))

(fn InitState
  (params (Target :type Actor%20Object%20Reference) (StateName :type Byte :default 0) (Commander :type BP%20State%20Commander%20Object%20Reference))
  (|CallParentFunction Target StateName Commander)
  (bind _returnvalue (CallFunction|AddComponent Target))
  (bind _output_get (Variables|Default|SetBPC_GetHideout _returnvalue))
  (Default|Initialize _output_get (Variables|/Game/Blueprints/AI/Pawn/BP_CreatureGeneric.BP_CreatureGeneric_C|GetDetectionArea (Variables|Default|GetSelfCreature)))
  (EventDispatchers|BindEventtoEDonHideoutLeaved _output_get (EventDispatchers|CreateEvent :!event Custom|ED_OnHideoutLeaved_Event))
  (EventDispatchers|BindEventtoEDonHideoutReached _output_get (EventDispatchers|CreateEvent :!event Custom|ED_OnHideoutReached_Event)))

(fn UseSkill
  (bind _bpc_gethideout (Variables|Default|GetBPC_GetHideout))
  (Default|AddDirection (Variables|/Game/Blueprints/AI/Pawn/BP_CreatureGeneric.BP_CreatureGeneric_C|GetBPC_ActorPhysicsMovement (Variables|Default|GetSelfCreature)) (* (Default|GetNearestHideoutDirection _bpc_gethideout) 5e+01))
  (Development|PrintText 0 (Utilities|Text|FormatText "Hideout Target : {x}" (Utilities|GetDisplayName (Default|GetNearestHideout _bpc_gethideout))) true true "(R=1.000000,G=0.480711,B=0.000000,A=1.000000)" 0.0)
  (|CallParentFunction))

(fn AddComponent
  (params (Target :type Actor%20Object%20Reference))
  (bind _output_get (LocalVariables|SetCurrentBPC (Actor|GetComponentbyClass Target "/Game/Blueprints/AddOn/Components/BPC_GetHideout.BPC_GetHideout_C")))
  (Utilities|IsValid _output_get
    (:Is%20Valid
      _)
    (:Is%20Not%20Valid
      (bind _returnvalue (Game|AddComponentbyClass Target "/Game/Blueprints/AddOn/Components/BPC_GetHideout.BPC_GetHideout_C"))
      (LocalVariables|SetCurrentBPC _returnvalue)))
  (return (LocalVariables|GetCurrentBPC)))