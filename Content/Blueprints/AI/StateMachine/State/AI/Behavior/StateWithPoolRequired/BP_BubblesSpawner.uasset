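; BP_BubblesSpawner is an AI behavior skill state that makes a creature release a pooled bubble behind itself.
; InitState registers bubble parameters, capping size at the creature's Size and deriving the rear gap from its sphere radius plus that maximum.
; When the skill is available, it launches a pool actor along the skeletal mesh's backward vector at that gap, passes the parameters, then marks the skill unavailable.
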(event EventWhileSkillAvailableEvent
  (params (DeltaTime :type Float%20%28double-precision%29))
  (CallFunction|UseSkill)
  (CallFunction|SetSkillAvailable false))

(fn UseSkill
  (bind _selfcreature (Variables|Default|GetSelfCreature))
  (bind _returnvalue (Transformation|GetActorTransform _selfcreature))
  (Default|LaunchPoolActor (Variables|/Game/Blueprints/AddOn/Components/BPC_PoolActorSpawner.BPC_PoolActorSpawner_C|GetPool (Variables|Default|GetBPCPool)) (Math|Transform|MakeTransform (+ (.location _returnvalue) (* (Default|GetParambyName (Variables|Default|GetBPC_Params) "GapMin") (Math|Vector|NegateVector (Math|Vector|GetForwardVector (Variables|/Game/Blueprints/AI/Pawn/BP_CreatureGeneric.BP_CreatureGeneric_C|GetSKM_Creature (Variables|Default|GetSelfCreature)))))) (.rotation _returnvalue)) (Variables|/Game/Blueprints/AddOn/Components/GenericComponents/BPC_ParamsByString.BPC_ParamsByString_C|GetParams (Variables|Default|GetBPC_Params)))
  (|CallParentFunction))

(fn InitState
  (params (Target :type Actor%20Object%20Reference) (StateName :type Byte :default 0) (Commander :type BP%20State%20Commander%20Object%20Reference))
  (|CallParentFunction Target StateName Commander)
  (Default|AddParamswithModify (Variables|Default|GetBPC_Params) (Utilities|Map|MakeMap "SizeMin" 1e+01 "SizeMax" (Utilities|Struct|BreakS_AICreatureStatSettings (.CreatureStatSettings (Utilities|Struct|BreakS_CreatureDetailsInstanced (Variables|/Game/Blueprints/AI/Pawn/BP_CreatureGeneric.BP_CreatureGeneric_C|GetUserData (Variables|Default|GetSelfCreature))))) "TimeBeforeDestroy" 5e+01 "PercentDamping" 0.6))
  (Default|AddParamswithModify (Variables|Default|GetBPC_Params) (Utilities|Map|MakeMap "GapMin" (+ (+ (Variables|/Script/Engine.SphereComponent|GetSphereRadius (Variables|/Game/Blueprints/AI/Pawn/BP_CreatureGeneric.BP_CreatureGeneric_C|GetRoot (Variables|Default|GetSelfCreature))) (Default|GetParambyName (Variables|Default|GetBPC_Params) "SizeMax")) 1.0))))