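; BP_AnchorSimple is a creature AI behavior state in the state machine that manages the creature's anchors.
; When the all-behaviors on/off event fires, it resets all anchors and enables their overlaps through the anchor manager, then calls the parent.
; The anchor manager's overlap-activation event sets the plunge material on a creature Niagara system via the VFX manager.
; Its update prints debug text showing overlappable, active and hookable anchor status.
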(event EventCreatureonOFFAllBehaviorsEvent
  (params (Active :type Boolean))
  (bind _bpc_anchormanager (Variables|Default|GetBPC_AnchorManager))
  (Default|ResetAllAnchor _bpc_anchormanager)
  (Default|SetActiveAllOverlapAnchors _bpc_anchormanager true)
  (|CallParentFunction Active)
  (Development|PrintText 0 "WOOOOOW!!!!!!!!!!!!" true true "(R=0.199721,G=1.000000,B=0.028119,A=1.000000)" 1e+01))

(event EventBPCAnchorEDonActiveAllOverlapEvent
  (Default|SetMaterialNiagaraSystem (Variables|/Game/Blueprints/AI/Pawn/BP_CreatureGeneric.BP_CreatureGeneric_C|GetBPC_VFX_Manager (Variables|Default|GetSelfCreature)) "NewEnumerator1" "Material" "/Game/VFX/Materials/Fish/M_Plunge.M_Plunge"))

(event EventIUpdate
  (params (DeltaSeconds :type Float%20%28double-precision%29))
  (bind _bpc_anchormanager (Variables|Default|GetBPC_AnchorManager))
  (|CallParentFunction DeltaSeconds)
  (Development|PrintText 0 (Utilities|Text|FormatText "------------------------ 
Anchor Overlapable  {x} 
Has Anchor Active {y} 
Has Anchor Hookable {z}" (Variables|/Game/Blueprints/AddOn/Components/BPC_AnchorManager.BPC_AnchorManager_C|GetAreAnchorOverlappeable _bpc_anchormanager) (Default|HasAnchorActive _bpc_anchormanager) (.HasAnyAnchorActive (Default|HasAnchorHookeable _bpc_anchormanager))) true true "(R=0.226958,G=1.000000,B=0.151697,A=1.000000)" 0.0))