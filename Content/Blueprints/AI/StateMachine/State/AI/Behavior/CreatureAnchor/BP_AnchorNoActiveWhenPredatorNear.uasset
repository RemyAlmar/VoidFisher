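; Creature anchor AI behavior state that, as its name indicates, disables anchors when a predator is near.
; When the inherited can-use-skill value changes, it sets all overlapping anchors through BPCAnchorManager to the opposite state.
; The same change fires the creature's use or stop skill dispatcher and recolors its Niagara sprite magenta or cyan.
; Any activation event re-enables the overlapping anchors; the update is empty, and detection is not in this graph.
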(event EventIUpdate
  (params (DeltaSeconds :type Float%20%28double-precision%29)))

(event EventOnCanUseValueChangedEvent
  (params (CanUseSkill :type Boolean))
  (bind _selfcreature (Variables|Default|GetSelfCreature))
  (Default|ActiveAllOverlapAnchors (Variables|Default|GetBPC_AnchorManager) (not CanUseSkill))
  (if CanUseSkill
    (Default|CallEDonUseSkill _selfcreature)
    (Default|SetColorNiagaraSystem (Variables|/Game/Blueprints/AI/Pawn/BP_CreatureGeneric.BP_CreatureGeneric_C|GetBPC_VFX_Manager (Variables|Default|GetSelfCreature)) "NewEnumerator1" "SpriteColor" "(R=5.000000,G=0.000000,B=1.450226,A=1.000000)")
    (else
      (Default|CallEDonStopSkill _selfcreature)
      (Default|SetColorNiagaraSystem (Variables|/Game/Blueprints/AI/Pawn/BP_CreatureGeneric.BP_CreatureGeneric_C|GetBPC_VFX_Manager (Variables|Default|GetSelfCreature)) "NewEnumerator1" "SpriteColor" "(R=0.000000,G=3.305063,B=5.000000,A=1.000000)"))))

(event EventEDonActivateEvent
  (params (Active :type Boolean))
  (Default|ActiveAllOverlapAnchors (Variables|Default|GetBPC_AnchorManager) true)
  (|CallParentFunction Active))

(fn InitState
  (params (Target :type Actor%20Object%20Reference) (StateName :type Byte :default 0) (Commander :type BP%20State%20Commander%20Object%20Reference))
  (|CallParentFunction Target StateName Commander))

(fn UseSkill
  (|CallParentFunction))