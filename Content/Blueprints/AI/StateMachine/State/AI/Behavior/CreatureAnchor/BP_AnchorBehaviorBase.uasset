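; Base AI behavior state for creatures protected by hookable anchors, making them catchable only when no anchor remains active.
; On init it binds to the creature's anchor manager, scales anchor radius by creature size and activates all anchors.
; Hook attach records a timecode and subscribes to the hook's event, left empty here; detach rechecks anchors to update catchability.
; Timecode difference helpers are included, though the seconds version multiplies hours by 360.
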(event Custom|BPC_Anchor_ED_OnDetachHook_Event
  (bind _hookactuallyon (Variables|Default|GetHookActuallyOn)
    (:then
      (EventDispatchers|UnbindEventfromEDCurrentlyHooked _hookactuallyon (EventDispatchers|CreateEvent :!event Custom|BPC_Hook_ED_OnCurrentHooked_Event)))
    (:else
      _))
  (Variables|Default|SetHookActuallyOn 0)
  (if (not (.HasAnyAnchorActive (Default|HasAnchorActive (Variables|Default|GetBPC_AnchorManager))))
    (CallFunction|OnAllAnchorDeactivate)))

(event Custom|BPCAnchor_ED_OnAttachHook_Event
  (Variables|Default|SetTimeHooked (Class|TimeManagementBlueprintLibrary|GetTimecode))
  (bind _bpc_anchormanager (Variables|Default|GetBPC_AnchorManager)
    (:then
      (bind _hookcomp (Variables|/Game/Blueprints/AddOn/Components/BPC_AnchorManager.BPC_AnchorManager_C|GetHookComp _bpc_anchormanager)
        (:then
          (bind _output_get (Variables|Default|SetHookActuallyOn _hookcomp))
          (EventDispatchers|BindEventtoEDCurrentlyHooked _output_get (EventDispatchers|CreateEvent :!event Custom|BPC_Hook_ED_OnCurrentHooked_Event)))
        (:else)))
    (:else)))

(event Custom|OnAllAnchorDeactivate
  (Default|SetIsCatcheable (Variables|Default|GetSelfCreature) (not (.HasAnyAnchorActive (Default|HasAnchorActive (Variables|Default|GetBPC_AnchorManager))))))

(event Custom|BPC_Hook_ED_OnCurrentHooked_Event)

(fn InitState
  (params (Target :type Actor%20Object%20Reference) (StateName :type Byte :default 0) (Commander :type BP%20State%20Commander%20Object%20Reference))
  (|CallParentFunction Target StateName Commander)
  (bind _asbpc_anchor_manager (Utilities|Casting|CastToBPC_AnchorManager (CallFunction|TryGetComponent (Variables|Default|GetSelfCreature) "/Game/Blueprints/AddOn/Components/BPC_AnchorManager.BPC_AnchorManager_C"))
    (:then
      (bind _output_get (Variables|Default|SetBPC_AnchorManager _asbpc_anchor_manager))
      (EventDispatchers|BindEventtoEDonAttachHook _output_get (EventDispatchers|CreateEvent :!event Custom|BPCAnchor_ED_OnAttachHook_Event))
      (EventDispatchers|BindEventtoEDonDetachHook _output_get (EventDispatchers|CreateEvent :!event Custom|BPC_Anchor_ED_OnDetachHook_Event))
      (Default|SetAnchorRadius (Variables|Default|GetBPC_AnchorManager) (* (.Size (Utilities|Struct|BreakS_AICreatureStatSettings (Utilities|Struct|BreakS_CreatureDetailsInstanced (Variables|/Game/Blueprints/AI/Pawn/BP_CreatureGeneric.BP_CreatureGeneric_C|GetUserData (Variables|Default|GetSelfCreature))))) 3e+02))
      (Default|ActiveAllAnchors (Variables|Default|GetBPC_AnchorManager) true)
      (Default|SetIsCatcheable (Variables|Default|GetSelfCreature) (not (.HasAnyAnchorActive (Default|HasAnchorActive (Variables|Default|GetBPC_AnchorManager))))))
    (:CastFailed
      (Development|PrintText 0 "Echec creation Anchor Component"))))

(fn GetDifferenceTime
  (params (PreTime :type Timecode%20Structure%20%28by%20ref%29) (CurTime :type Timecode%20Structure%20%28by%20ref%29))
  (bind (_hours _minutes _seconds) (Utilities|Struct|BreakTimecode CurTime))
  (bind (_hours_2 _minutes_2 _seconds_2) (Utilities|Struct|BreakTimecode PreTime))
  (LocalVariables|SetTimePassed (Utilities|Struct|MakeTimecode (- _hours _hours_2) (- _minutes _minutes_2) (- _seconds _seconds_2) 0 false))
  (return (LocalVariables|GetTimePassed)))

(fn GetDifferenceMinute
  (params (PreTime :type Timecode%20Structure%20%28by%20ref%29) (CurTime :type Timecode%20Structure%20%28by%20ref%29))
  (bind _output_get (Time|GetDifferenceTime PreTime CurTime))
  (bind (_hours _minutes) (Utilities|Struct|BreakTimecode _output_get))
  (return (+ (* _hours 60) _minutes)))

(fn GetDifferenceSecond
  (params (PreTime :type Timecode%20Structure%20%28by%20ref%29) (CurTime :type Timecode%20Structure%20%28by%20ref%29))
  (bind _output_get (Time|GetDifferenceTime PreTime CurTime))
  (bind (_hours _minutes _seconds) (Utilities|Struct|BreakTimecode _output_get))
  (return (+ (+ (* _hours 360) (* _minutes 60)) _seconds)))