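; Creature AI behavior state that protects a creature's anchors with a spherical shield that only a dash can break.
; On init it sizes the creature's BPC_Shield from its root sphere, enables CCD and disables overlap anchors.
; A hit from an actor mid-dash makes the skill unavailable.
; Cooldown start drops the shield and enables the anchors; cooldown reset reverses this, and quitting deactivates the shield.
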(event Custom|ED_OnHitCollision_Event
  (params (HitComponent :type Primitive%20Component%20Object%20Reference) (OtherActor :type Actor%20Object%20Reference) (OtherComp :type Primitive%20Component%20Object%20Reference) (NormalImpulse :type Vector) (Hit :type Hit%20Result%20Structure%20%28by%20ref%29))
  (bind _returnvalue (Actor|GetComponentbyClass OtherActor "/Game/Blueprints/AddOn/Components/BPC_Dash.BPC_Dash_C"))
  (Utilities|IsValid _returnvalue
    (:Is%20Valid
      (if (Variables|/Game/Blueprints/AddOn/Components/BPC_Dash.BPC_Dash_C|GetIsInDash _returnvalue)
        (CallFunction|SetSkillAvailable false)))))

(event EventIQuit
  (|CallParentFunction)
  (Default|DeactiveShield (Variables|Default|GetBPC%20Shield)))

(event EventIUpdate
  (params (DeltaSeconds :type Float%20%28double-precision%29))
  (|CallParentFunction DeltaSeconds)
  (Default|SetMaterialOpacity (Variables|Default|GetBPC%20Shield) 0.0 true))

(event EventEDonCooldownStartEvent
  (|CallParentFunction)
  (Default|ActiveAllOverlapAnchors (Variables|Default|GetBPC_AnchorManager) true)
  (Default|SetActiveShield (Variables|Default|GetBPC%20Shield) false))

(event EventEDonCooldownResetEvent
  (|CallParentFunction)
  (Default|ActiveAllOverlapAnchors (Variables|Default|GetBPC_AnchorManager) false)
  (Default|SetActiveShield (Variables|Default|GetBPC%20Shield) true))

(fn InitState
  (params (Target :type Actor%20Object%20Reference) (StateName :type Byte :default 0) (Commander :type BP%20State%20Commander%20Object%20Reference))
  (bind _selfcreature (Variables|Default|GetSelfCreature))
  (|CallParentFunction Target StateName Commander)
  (bind _asbpc_shield (Utilities|Casting|CastToBPC_Shield (CallFunction|TryGetComponent _selfcreature "/Game/Blueprints/AddOn/Components/BPC_Shield.BPC_Shield_C")))
  (bind _output_get (Variables|Default|SetBPC%20Shield _asbpc_shield))
  (Default|Init _output_get (+ (Variables|/Script/Engine.SphereComponent|GetSphereRadius (Variables|/Game/Blueprints/AI/Pawn/BP_CreatureGeneric.BP_CreatureGeneric_C|GetRoot _selfcreature)) 1.5e+02) "/Engine/EngineMeshes/Sphere.Sphere" (+ (Math|Vector|GetMaxElement (Transformation|GetWorldScale (Variables|/Game/Blueprints/AI/Pawn/BP_CreatureGeneric.BP_CreatureGeneric_C|GetSKM_Creature (Variables|Default|GetSelfCreature)))) 3.0) false)
  (Variables|/Game/Blueprints/AddOn/Components/BPC_Shield.BPC_Shield_C|SetIsHidden _output_get true)
  (EventDispatchers|BindEventtoEDonCollisionHit _output_get (EventDispatchers|CreateEvent :!event Custom|ED_OnHitCollision_Event))
  (Default|SetActiveShield (Variables|Default|GetBPC%20Shield) true)
  (Default|ActiveAllOverlapAnchors (Variables|Default|GetBPC_AnchorManager) false)
  (Class|PrimitiveComponent|SetUseCCD (Variables|/Game/Blueprints/AddOn/Components/BPC_Shield.BPC_Shield_C|GetShieldCollision (Variables|Default|GetBPC%20Shield)) true "None"))