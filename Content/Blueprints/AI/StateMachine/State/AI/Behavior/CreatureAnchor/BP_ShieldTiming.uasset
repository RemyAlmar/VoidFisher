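; BP_ShieldTiming is a creature AI behavior state that alternates a timed shield with the creature's anchors.
; On init it finds the creature's BPC_Shield and sizes it, hidden, from the creature's root sphere and mesh scale.
; Skill availability toggles the shield on and overlap anchors off, or the reverse, and a timer ends each available window.
; Each update drives shield opacity toward zero, and quitting deactivates the shield.
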(event EventIQuit
  (|CallParentFunction)
  (Default|DeactiveShield (Variables|Default|GetBPC%20Shield)))

(event EventIUpdate
  (params (DeltaSeconds :type Float%20%28double-precision%29))
  (|CallParentFunction DeltaSeconds)
  (Default|SetMaterialOpacity (Variables|Default|GetBPC%20Shield) 0.0 true))

(event EventWhileSkillAvailableEvent
  (params (DeltaTime :type Float%20%28double-precision%29))
  (if (CallFunction|TimerPos (Variables|Default|GetShieldActiveCurrentTime) DeltaTime 1e+01 true)
    (CallFunction|SetSkillAvailable false)))

(event EventOnSkillAvailableValueChangedEvent
  (params (SkillAvailable :type Boolean))
  (Default|ActiveAllOverlapAnchors (Variables|Default|GetBPC_AnchorManager) (not SkillAvailable))
  (Default|SetActiveShield (Variables|Default|GetBPC%20Shield) SkillAvailable))

(fn InitState
  (params (Target :type Actor%20Object%20Reference) (StateName :type Byte :default 0) (Commander :type BP%20State%20Commander%20Object%20Reference))
  (bind _selfcreature (Variables|Default|GetSelfCreature))
  (|CallParentFunction Target StateName Commander)
  (bind _asbpc_shield (Utilities|Casting|CastToBPC_Shield (CallFunction|TryGetComponent _selfcreature "/Game/Blueprints/AddOn/Components/BPC_Shield.BPC_Shield_C")))
  (bind _output_get (Variables|Default|SetBPC%20Shield _asbpc_shield))
  (Default|Init _output_get (+ (Variables|/Script/Engine.SphereComponent|GetSphereRadius (Variables|/Game/Blueprints/AI/Pawn/BP_CreatureGeneric.BP_CreatureGeneric_C|GetRoot _selfcreature)) 1.5e+02) "/Engine/EngineMeshes/Sphere.Sphere" (+ (Math|Vector|GetMaxElement (Transformation|GetWorldScale (Variables|/Game/Blueprints/AI/Pawn/BP_CreatureGeneric.BP_CreatureGeneric_C|GetSKM_Creature (Variables|Default|GetSelfCreature)))) 3.0) false)
  (Variables|/Game/Blueprints/AddOn/Components/BPC_Shield.BPC_Shield_C|SetIsHidden _output_get true))