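; Creature AI behavior state that gives the creature a timed water shield skill, toggling its overlap anchors inversely to the shield.
; InitState spawns a collision sphere sized from the creature's root and a mesh with a dynamic shield material.
; Skill availability switches collision, visibility and anchors, and a timer ends it, while IUpdate interpolates the material's Alpha to fade the effect.
; Quitting the state, noted as a stun, clears the shield immediately.
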(event EventIQuit
  ;[0.5431 1 0.4301] it's Stun
  (|CallParentFunction)
  (Rendering|Material|SetScalarParameterValue (Variables|Default|GetMID_Shield) "Alpha" 0.0 :!class /Script/Engine.MaterialInstanceDynamic)
  (Collision|SetCollisionProfileName (Variables|Default|GetShieldCollision) "NoCollision" true :!class /Script/Engine.PrimitiveComponent)
  (Development|SetHiddeninGame (Variables|Default|GetShieldCollision) true false) ; Affiche/ Desaffiche le shield
)

(event EventIUpdate
  (params (DeltaSeconds :type Float%20%28double-precision%29))
  (bind _mid_shield (Variables|Default|GetMID_Shield))
  (bind _mid_shield_2 (Variables|Default|GetMID_Shield))
  (|CallParentFunction DeltaSeconds)
  (if (Variables|Default|GetIsActive)
    ;[0.6457 1 0.9901] FadeShieldVFx
    (bind _returnvalue (Rendering|Material|GetScalarParameterValue _mid_shield_2 "Alpha" :!class /Script/Engine.MaterialInstanceDynamic))
    (Rendering|Material|SetScalarParameterValue _mid_shield_2 "Alpha" (Math|Interpolation|FInterpTo _returnvalue 1.0 DeltaSeconds 1.0) :!class /Script/Engine.MaterialInstanceDynamic)
    (else
      (bind _returnvalue_2 (Rendering|Material|GetScalarParameterValue _mid_shield "Alpha" :!class /Script/Engine.MaterialInstanceDynamic))
      (Rendering|Material|SetScalarParameterValue _mid_shield "Alpha" (Math|Interpolation|FInterpTo _returnvalue_2 0.0 DeltaSeconds 1.0) :!class /Script/Engine.MaterialInstanceDynamic)))
  (Development|PrintText 0 (Utilities|Text|FormatText "Cooldown {x} / {y} 
Skill Available {z}" (Variables|Default|GetCurrentTime) (Variables|Default|GetCooldownMax) (Variables|Default|GetSkill%20Available)) true true "(R=1.000000,G=0.466324,B=0.000000,A=1.000000)" 0.0))

(event EventWhileSkillAvailableEvent
  (params (DeltaTime :type Float%20%28double-precision%29))
  (if (CallFunction|TimerPos (Variables|Default|GetShieldActiveCurrentTime) DeltaTime 1e+01 true)
    (CallFunction|SetSkillAvailable false)))

(event EventOnSkillAvailableValueChangedEvent
  (params (SkillAvailable :type Boolean))
  (bind _returnvalue (not SkillAvailable))
  (bind _shieldcollision (Variables|Default|GetShieldCollision))
  (Default|ActiveAllOverlapAnchors (Variables|Default|GetBPC_AnchorManager) _returnvalue)
  (bind _output_get (Variables|Default|SetIsActive SkillAvailable))
  (if _output_get
    (Collision|SetCollisionProfileName (Variables|Default|GetShieldCollision) "Shield" true :!class /Script/Engine.PrimitiveComponent)
    (else
      (Collision|SetCollisionProfileName (Variables|Default|GetShieldCollision) "NoCollision" false :!class /Script/Engine.PrimitiveComponent)))
  (Development|SetHiddeninGame _shieldcollision _returnvalue true) ; Affiche/ Desaffiche le shield
  (Development|PrintText 0 (Utilities|Text|FormatText "Has {x } as collision name 
Shield Activated {y}" (Collision|GetCollisionProfileName _shieldcollision) (Variables|Default|GetIsActive)) true true "(R=0.000000,G=1.000000,B=0.138758,A=1.000000)" 5.0))

(fn InitState
  (params (Target :type Actor%20Object%20Reference) (StateName :type Byte :default 0) (Commander :type BP%20State%20Commander%20Object%20Reference))
  (bind _selfcreature (Variables|Default|GetSelfCreature))
  (bind _selfcreature_2 (Variables|Default|GetSelfCreature))
  (bind _root (Variables|/Game/Blueprints/AI/Pawn/BP_CreatureGeneric.BP_CreatureGeneric_C|GetRoot _selfcreature_2))
  (|CallParentFunction Target StateName Commander)
  (bind _returnvalue (Rendering|Material|CreateDynamicMaterialInstance _selfcreature_2 "/Game/VFX/Materials/Fish/M_WaterShield.M_WaterShield" "None" :!class /Script/Engine.KismetMaterialLibrary))
  (Variables|Default|SetMID_Shield _returnvalue)
  (bind _returnvalue_2 (Default|CreateSphere _selfcreature_2 (+ (Variables|/Script/Engine.SphereComponent|GetSphereRadius _root) 5e+01) true "NoCollision"))
  (bind _output_get (Variables|Default|SetShieldCollision _returnvalue_2))
  (Transformation|AttachComponentToComponent _output_get _root "None" "KeepRelative" "KeepRelative" "KeepRelative" true)
  (bind _returnvalue_3 (Default|CreateStaticMesh _selfcreature "/Engine/EngineMeshes/Sphere.Sphere" (Variables|Default|GetMID_Shield) (+ (Math|Vector|GetMaxElement (Transformation|GetWorldScale (Variables|/Game/Blueprints/AI/Pawn/BP_CreatureGeneric.BP_CreatureGeneric_C|GetSKM_Creature _selfcreature))) 2.0) "0, 0, 0" "0, 0, 0"))
  (Collision|SetCollisionProfileName _returnvalue_3 "NoCollision" false :!class /Script/Engine.PrimitiveComponent)
  (Rendering|Material|SetScalarParameterValue (Variables|Default|GetMID_Shield) "Alpha" 0.0 :!class /Script/Engine.MaterialInstanceDynamic))