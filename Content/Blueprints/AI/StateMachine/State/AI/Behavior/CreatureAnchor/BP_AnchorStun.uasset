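; Creature anchor behavior state that stuns the creature once all of its hook anchors are deactivated.
; While an anchor has been hooked for over three seconds, it switches off that anchor's sphere collision through the anchor manager.
; When all anchors are deactivated, it adds and immediately starts a BP_Stunned state on the creature's movement state manager.
; Attach and detach hook events only call the parent logic.
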(event EventBPCAnchorEDonAttachHookEvent
  (|CallParentFunction))

(event EventBPCAnchorEDonDetachHookEvent
  (|CallParentFunction))

(event EventBPCHookEDonCurrentHookedEvent
  (bind _bpc_anchormanager (Variables|Default|GetBPC_AnchorManager))
  (|CallParentFunction)
  (if (> (CallFunction|GetDifferenceSecond (Variables|Default|GetTimeHooked) (Class|TimeManagementBlueprintLibrary|GetTimecode)) 3.0)
    (Default|ActiveSphereCollision _bpc_anchormanager (Variables|/Game/Blueprints/AddOn/Components/BPC_AnchorManager.BPC_AnchorManager_C|GetCurrentAnchorHooked _bpc_anchormanager) false)))

(event EventOnAllAnchorDeactivate
  (|CallParentFunction)
  (Default|AddState (Variables|/Game/Blueprints/AI/Pawn/BP_CreatureGeneric.BP_CreatureGeneric_C|GetBPC_StateManager_Movement (Variables|Default|GetSelfCreature)) (Utilities|Enum|LiteralenumE_StateMovement "NewEnumerator3") true "/Game/Blueprints/AI/StateMachine/State/AI/Movement/BP_Stunned.BP_Stunned_C"))