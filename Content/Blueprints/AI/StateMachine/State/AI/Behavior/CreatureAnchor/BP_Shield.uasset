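; Creature AI behavior state that gives an anchor creature a water shield, a collision sphere plus dynamic-material mesh built in InitState.
; While the skill is available the shield blocks and fades in; a fixed timer then makes it unavailable.
; That change drops shield collision, activates overlapping anchors through BPCAnchorManager and fades the material out.
; Quitting the state, noted as a stun, clears the shield immediately.
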(event EventIQuit
  ;[0.5431 1 0.4301] it's Stun
  (|CallParentFunction)
  (Rendering|Material|SetScalarParameterValue (Variables|Default|GetMID_Shield) "Alpha" 0.0 :!class /Script/Engine.MaterialInstanceDynamic)
  (Collision|SetCollisionProfileName (Variables|Default|GetShieldCollision) "NoCollision" true :!class /Script/Engine.PrimitiveComponent)
  (Development|SetHiddeninGame (Variables|Default|GetShieldCollision) true false) ; Affiche/ Desaffiche le shield
)

(event EventIUpdate
  (params (DeltaSeconds :type Float%20%28double-precision%29))
  (bind _mid_shield (Variables|Default|GetMID_Shield))
  (bind _mid_shield_2 (Variables|Default|GetMID_Shield))
  (|CallParentFunction DeltaSeconds)
  (if (Variables|Default|GetIsActive)
    ;[0.6457 1 0.9901] FadeShieldVFx
    (bind _returnvalue (Rendering|Material|GetScalarParameterValue _mid_shield_2 "Alpha" :!class /Script/Engine.MaterialInstanceDynamic))
    (Rendering|Material|SetScalarParameterValue _mid_shield_2 "Alpha" (Math|Interpolation|FInterpTo _returnvalue 0.0 DeltaSeconds 1.0) :!class /Script/Engine.MaterialInstanceDynamic)
    (else
      (bind _returnvalue_2 (Rendering|Material|GetScalarParameterValue _mid_shield "Alpha" :!class /Script/Engine.MaterialInstanceDynamic))
      (Rendering|Material|SetScalarParameterValue _mid_shield "Alpha" (Math|Interpolation|FInterpTo _returnvalue_2 1.0 DeltaSeconds 1.0) :!class /Script/Engine.MaterialInstanceDynamic))))

(event EventWhileSkillAvailableEvent
  (params (DeltaTime :type Float%20%28double-precision%29))
  (CallFunction|SetSkillAvailable (not (CallFunction|TimerPos (Variables|Default|GetShieldActiveCurrentTime) DeltaTime 7.0 true)))
  (|CallParentFunction DeltaTime))

(event EventEDonCooldownResetEvent
  (CallFunction|SetStartCooldown false)
  (|CallParentFunction))

(event EventOnSkillAvailableValueChangedEvent
  (params (SkillAvailable :type Boolean))
  (bind _returnvalue (not SkillAvailable))
  (Default|ActiveAllOverlapAnchors (Variables|Default|GetBPC_AnchorManager) _returnvalue)
  (Variables|Default|SetIsActive _returnvalue)
  (if _returnvalue
    (Collision|SetCollisionProfileName (Variables|Default|GetShieldCollision) "NoCollision" true :!class /Script/Engine.PrimitiveComponent)
    (else
      (Collision|SetCollisionProfileName (Variables|Default|GetShieldCollision) "Shield" true :!class /Script/Engine.PrimitiveComponent)))
  (Development|SetHiddeninGame (Variables|Default|GetShieldCollision) true false) ; Affiche/ Desaffiche le shield
)

(fn InitState
  (params (Target :type Actor%20Object%20Reference) (StateName :type Byte :default 0) (Commander :type BP%20State%20Commander%20Object%20Reference))
  (bind _selfcreature (Variables|Default|GetSelfCreature))
  (|CallParentFunction Target StateName Commander)
  (bind _returnvalue (Rendering|Material|CreateDynamicMaterialInstance _selfcreature "/Game/VFX/Materials/Fish/M_WaterShield.M_WaterShield" "None" :!class /Script/Engine.KismetMaterialLibrary))
  (bind _output_get (Variables|Default|SetMID_Shield _returnvalue))
  (bind _returnvalue_2 (Default|CreateSphere _selfcreature (Variables|/Script/Engine.SphereComponent|GetSphereRadius (Variables|/Game/Blueprints/AI/Pawn/BP_CreatureGeneric.BP_CreatureGeneric_C|GetRoot _selfcreature)) true))
  (Variables|Default|SetShieldCollision _returnvalue_2)
  (bind _returnvalue_3 (Default|CreateStaticMesh _selfcreature "/Engine/EngineMeshes/Sphere.Sphere" _output_get (+ (Math|Vector|GetMaxElement (Transformation|GetWorldScale (Variables|/Game/Blueprints/AI/Pawn/BP_CreatureGeneric.BP_CreatureGeneric_C|GetSKM_Creature _selfcreature))) 2.0) "0, 0, 0" "0, 0, 0"))
  (Collision|SetCollisionEnabled _returnvalue_3 "NoCollision")
  (Rendering|Material|SetScalarParameterValue (Variables|Default|GetMID_Shield) "Alpha" 0.0 :!class /Script/Engine.MaterialInstanceDynamic))