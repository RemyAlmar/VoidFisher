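; Base AI state machine behavior for prey creatures that adjusts movement speed and skill availability in response to predators.
; On init it binds handlers to the creature's BPCPrey event dispatchers.
; A predator reaction sets prey speed from AI data, and losing all predators restores neutral speed.
; Skill use is re-evaluated against nearby predators when one is seen or none remain; afraid, aimed and predator-out handlers are empty.
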(event Custom|BPC_Prey_ED_SeePredatorInRange
  (params (TargetPredator :type Actor%20Object%20Reference))
  (CallFunction|SetCanUseSkill (Default|HasPredatorNear (Variables|/Game/Blueprints/AI/Pawn/BP_CreatureGeneric.BP_CreatureGeneric_C|GetBPC_Prey (Variables|Default|GetSelfCreature)) (CallFunction|GetRangeDistance))))

(event Custom|BPC_Prey_ED_IsAfraid_Event)

(event Custom|BPC_Prey_ED_IsAimed_Event)

(event Custom|BPC_Prey_ED_WithoutPredator_Event
  (CallFunction|SetNeutralSpeed)
  (CallFunction|SetCanUseSkill (Default|HasPredatorNear (Variables|/Game/Blueprints/AI/Pawn/BP_CreatureGeneric.BP_CreatureGeneric_C|GetBPC_Prey (Variables|Default|GetSelfCreature)) (CallFunction|GetRangeDistance))))

(event Custom|BPC_Prey_ED_ReactOnPredatorOut
  (params (TargetPredator :type Actor%20Object%20Reference)))

(event Custom|BPC_Prey_ED_ReactOnPredatorIn
  (params (TargetPredator :type Actor%20Object%20Reference))
  (CallFunction|SetPreySpeed))

(fn InitState
  (params (Target :type Actor%20Object%20Reference) (StateName :type Byte :default 0) (Commander :type BP%20State%20Commander%20Object%20Reference))
  (bind _selfcreature (Variables|Default|GetSelfCreature))
  (bind _bpc_prey (Variables|/Game/Blueprints/AI/Pawn/BP_CreatureGeneric.BP_CreatureGeneric_C|GetBPC_Prey _selfcreature))
  (|CallParentFunction Target StateName Commander)
  (EventDispatchers|BindEventtoEDReactonPredatorin _bpc_prey (EventDispatchers|CreateEvent :!event Custom|BPC_Prey_ED_ReactOnPredatorIn))
  (EventDispatchers|BindEventtoEDReactonPredatorOut _bpc_prey (EventDispatchers|CreateEvent :!event Custom|BPC_Prey_ED_ReactOnPredatorOut))
  (EventDispatchers|BindEventtoEDSeePredatorinRange _bpc_prey (EventDispatchers|CreateEvent :!event Custom|BPC_Prey_ED_SeePredatorInRange))
  (EventDispatchers|BindEventtoEDIsAimed _bpc_prey (EventDispatchers|CreateEvent :!event Custom|BPC_Prey_ED_IsAimed_Event))
  (EventDispatchers|BindEventtoEDIsWithoutPredator _bpc_prey (EventDispatchers|CreateEvent :!event Custom|BPC_Prey_ED_WithoutPredator_Event))
  (EventDispatchers|BindEventtoEDIsAfraid _bpc_prey (EventDispatchers|CreateEvent :!event Custom|BPC_Prey_ED_IsAfraid_Event)))

(fn SetPreySpeed
  (bind _selfcreature (Variables|Default|GetSelfCreature))
  (Variables|/Game/Blueprints/AddOn/Components/BPC_ActorPhysicsMovement.BPC_ActorPhysicsMovement_C|SetTargetSpeed (Variables|/Game/Blueprints/AI/Pawn/BP_CreatureGeneric.BP_CreatureGeneric_C|GetBPC_ActorPhysicsMovement _selfcreature) (.prey (Utilities|Struct|BreakS_AICreatureBehaviorSettings (Default|GetAIData _selfcreature))))
  (return))

(fn SetNeutralSpeed
  (bind _selfcreature (Variables|Default|GetSelfCreature))
  (Variables|/Game/Blueprints/AddOn/Components/BPC_ActorPhysicsMovement.BPC_ActorPhysicsMovement_C|SetTargetSpeed (Variables|/Game/Blueprints/AI/Pawn/BP_CreatureGeneric.BP_CreatureGeneric_C|GetBPC_ActorPhysicsMovement _selfcreature) (.neutre (Utilities|Struct|BreakS_AICreatureBehaviorSettings (Default|GetAIData _selfcreature))))
  (return))