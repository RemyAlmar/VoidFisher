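; AI behavior state that lets a creature open a wormhole ahead of itself and steer toward it.
; UseSkill closes any existing wormhole, spawns a new one scaled to the creature at twice its forward detection distance, then creates a randomized exit.
; Each update adds movement direction toward the active wormhole.
; InitState creates a visible, collision-free sphere sized from the detection radius and the state's normalized distance.
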(event EventIUpdate
  (params (DeltaSeconds :type Float%20%28double-precision%29))
  (bind _worm_hole (Variables|Default|GetWorm%20Hole)
    (:then
      (Default|AddDirection (Variables|/Game/Blueprints/AI/Pawn/BP_CreatureGeneric.BP_CreatureGeneric_C|GetBPC_ActorPhysicsMovement (Variables|Default|GetSelfCreature)) (Math|Vector|GetUnitDirection(Vector) (Transformation|GetActorLocation (Variables|Default|GetSelfCreature)) (Transformation|GetActorLocation _worm_hole))))
    (:else
      _))
  (|CallParentFunction DeltaSeconds))

(fn UseSkill
  (bind _selfcreature (Variables|Default|GetSelfCreature))
  (bind _selfcreature_2 (Variables|Default|GetSelfCreature))
  (bind _worm_hole (Variables|Default|GetWorm%20Hole)
    (:then
      (Default|OnCloseWormHole _worm_hole))
    (:else
      _))
  (bind _returnvalue (Default|SpawnSomething _selfcreature_2 "/Game/Blueprints/Game/Player/Spawnables/BP_WormHole.BP_WormHole_C" (Math|Transform|MakeTransform (+ (Transformation|GetActorLocation _selfcreature_2) (* (Transformation|GetActorForwardVector _selfcreature_2) (* (Utilities|Struct|BreakS_AICreatureBehaviorSettings (.CreatureBehaviorSettings (Utilities|Struct|BreakS_CreatureDetailsInstanced (Variables|/Game/Blueprints/AI/Pawn/BP_CreatureGeneric.BP_CreatureGeneric_C|GetUserData _selfcreature)))) 2.0))) (Transformation|GetActorRotation _selfcreature_2) (Transformation|GetWorldScale (Variables|/Game/Blueprints/AI/Pawn/BP_CreatureGeneric.BP_CreatureGeneric_C|GetSKM_Creature _selfcreature)))))
  (bind _asbp_worm_hole (Utilities|Casting|CastToBP_WormHole _returnvalue)
    (:then
      (bind _output_get (Variables|Default|SetWorm%20Hole _asbp_worm_hole))
      (Default|CreateExitWormHole _output_get (Math|Random|RandomFloatinRange 5e+03 2.5e+04))
      (|CallParentFunction))
    (:CastFailed
      (Development|PrintString 0 "Le BP_WormHole a fail le cast"))))

(fn InitState
  (params (Target :type Actor%20Object%20Reference) (StateName :type Byte :default 0) (Commander :type BP%20State%20Commander%20Object%20Reference))
  (bind _selfcreature (Variables|Default|GetSelfCreature))
  (|CallParentFunction Target StateName Commander)
  (Default|CreateSphere _selfcreature (* (Variables|/Script/Engine.SphereComponent|GetSphereRadius (Variables|/Game/Blueprints/AI/Pawn/BP_CreatureGeneric.BP_CreatureGeneric_C|GetDetectionArea _selfcreature)) (.Value (Utilities|Map|Find (Variables|/Game/Blueprints/AI/StateMachine/BP_StateCommander.BP_StateCommander_C|GetListDistanceNormalized Commander) StateName))) false "NoCollision"))