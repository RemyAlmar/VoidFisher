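; AI behavior state that spins a prey creature's skeletal mesh on its Z axis while a predator is near.
; When the skill manager switches it on, it binds to the prey component's predator-seen and no-predator events, unbinding when switched off.
; With a predator in range, it repeatedly adds a random, randomly signed rotation drawn from named creature parameters.
; Otherwise it interpolates the mesh rotation back, clearing the stored rotation once predators are gone.
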(event EventBPCPreyEDSeePredatorinRange
  (params (TargetPredator :type Actor%20Object%20Reference))
  (bind _selfcreature (Variables|Default|GetSelfCreature))
  (bind _skm_creature (Variables|/Game/Blueprints/AI/Pawn/BP_CreatureGeneric.BP_CreatureGeneric_C|GetSKM_Creature _selfcreature))
  (if (Default|HasPredatorNear (Variables|/Game/Blueprints/AI/Pawn/BP_CreatureGeneric.BP_CreatureGeneric_C|GetBPC_Prey (Variables|Default|GetSelfCreature)) (CallFunction|GetRangeDistance))
    (if (Utilities|Operators|EqualEqual :A (Variables|Default|GetTarget%20Rotation))
      (Variables|Default|SetTarget%20Rotation (Math|Rotator|MakeRotator 0.0 0.0 (* (Default|GetRandomFloatValueinRangebyParamName (Variables|/Game/Blueprints/AI/Pawn/BP_CreatureGeneric.BP_CreatureGeneric_C|GetBPC_ParamsByString (Variables|Default|GetSelfCreature)) "RotationMin" "RotationMax") (CallFunction|RandomSign)))))
    (Transformation|AddRelativeRotation _skm_creature (Variables|Default|GetTarget%20Rotation) false false)
    (else
      (Transformation|SetRelativeRotation _skm_creature (Math|Interpolation|RInterpTo (Variables|/Script/Engine.SceneComponent|GetRelativeRotation _skm_creature) "0, 0, 0" (Variables|Default|GetDeltaTime) 2.0) false false))))

(event EventBPCPreyEDonWithoutPredatorEvent
  (bind _selfcreature (Variables|Default|GetSelfCreature))
  (bind _skm_creature (Variables|/Game/Blueprints/AI/Pawn/BP_CreatureGeneric.BP_CreatureGeneric_C|GetSKM_Creature _selfcreature))
  (Transformation|SetRelativeRotation _skm_creature (Math|Interpolation|RInterpTo (Variables|/Script/Engine.SceneComponent|GetRelativeRotation _skm_creature) "0, 0, 0" (Variables|Default|GetDeltaTime) 2.0) false false)
  (Variables|Default|SetTarget%20Rotation "0, 0, 0"))

(event EventEDSkillManageronEvent
  (bind _selfcreature (Variables|Default|GetSelfCreature))
  (bind _bpc_prey (Variables|/Game/Blueprints/AI/Pawn/BP_CreatureGeneric.BP_CreatureGeneric_C|GetBPC_Prey _selfcreature))
  (EventDispatchers|BindEventtoEDSeePredatorinRange _bpc_prey (EventDispatchers|CreateEvent :!event BPCPreyEDSeePredatorinRange))
  (EventDispatchers|BindEventtoEDonWithoutPredator _bpc_prey (EventDispatchers|CreateEvent :!event BPCPreyEDonWithoutPredatorEvent)))

(event EventEDSkillManagerOffEvent
  (bind _selfcreature (Variables|Default|GetSelfCreature))
  (bind _bpc_prey (Variables|/Game/Blueprints/AI/Pawn/BP_CreatureGeneric.BP_CreatureGeneric_C|GetBPC_Prey _selfcreature))
  (EventDispatchers|UnbindEventfromEDSeePredatorinRange _bpc_prey (EventDispatchers|CreateEvent :!event BPCPreyEDSeePredatorinRange))
  (EventDispatchers|UnbindEventfromEDonWithoutPredator _bpc_prey (EventDispatchers|CreateEvent :!event BPCPreyEDonWithoutPredatorEvent)))

(fn RandomSign
  (if (Math|Random|RandomBool)
    _
    (else
      (Utilities|NegateInt (LocalVariables|GetCurrentSign)
        (:%20%20
          _))))
  (return (LocalVariables|GetCurrentSign)))