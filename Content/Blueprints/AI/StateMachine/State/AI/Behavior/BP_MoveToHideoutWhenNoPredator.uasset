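; AI behavior state that steers a prey creature to a known hideout when no predator is within range.
; It finds or adds a BPC_GetHideout component, and its skill feeds the nearest hideout direction into physics movement.
; Predator-out events update skill availability and the wish to hide, which drives placement in the hideout on update.
; Entering switches movement to idle, while a predator arriving restores AI movement and cancels hiding.
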(event Custom|ED_OnHideoutEnter_Event
  (params (Target :type BP%20Hideout%20Object%20Reference))
  (if (Variables|/Game/Blueprints/AddOn/Components/BPC_GetHideout.BPC_GetHideout_C|GetWantToHideSelf (Variables|Default|GetBPC_GetHideout))
    (Default|AddState (Variables|/Game/Blueprints/AI/Pawn/BP_CreatureGeneric.BP_CreatureGeneric_C|GetBPC_StateManager_Movement (Variables|Default|GetSelfCreature)) (Utilities|Enum|LiteralenumE_StateMovement "NewEnumerator0") true "/Game/Blueprints/AI/StateMachine/State/AI/Movement/BP_Idle.BP_Idle_C")))

(event Custom|ED_OnHideoutReached_Event
  (params (Target :type BP%20Hideout%20Object%20Reference)))

(event Custom|ED_OnHideoutLeaved_Event
  (params (Target :type BP%20Hideout%20Object%20Reference)))

(event EventBPCPreyEDReactonPredatorin
  (params (TargetPredator :type Actor%20Object%20Reference))
  (Default|AddState (Variables|/Game/Blueprints/AI/Pawn/BP_CreatureGeneric.BP_CreatureGeneric_C|GetBPC_StateManager_Movement (Variables|Default|GetSelfCreature)) (Utilities|Enum|LiteralenumE_StateMovement "NewEnumerator1") true "/Game/Blueprints/AI/StateMachine/State/AI/Movement/BP_MoveAI.BP_MoveAI_C")
  (Default|SetWanttoHideSelf (Variables|Default|GetBPC_GetHideout) false)
  (|CallParentFunction TargetPredator))

(event EventBPCPreyEDReactonPredatorOut
  (params (TargetPredator :type Actor%20Object%20Reference))
  (bind _returnvalue (CallFunction|GetRangeDistance))
  (bind _selfcreature (Variables|Default|GetSelfCreature))
  (bind _bpc_prey (Variables|/Game/Blueprints/AI/Pawn/BP_CreatureGeneric.BP_CreatureGeneric_C|GetBPC_Prey _selfcreature))
  (bind _predatornearout (Default|HasPredatorNear _bpc_prey _returnvalue))
  (bind _returnvalue_2 (not _predatornearout))
  (CallFunction|SetCanUseSkill (and (Default|HasHideoutKnown (Variables|Default|GetBPC_GetHideout)) _returnvalue_2))
  (Default|SetWanttoHideSelf (Variables|Default|GetBPC_GetHideout) _returnvalue_2))

(event EventIUpdate
  (params (DeltaSeconds :type Float%20%28double-precision%29))
  (bind _bpc_gethideout (Variables|Default|GetBPC_GetHideout))
  (if (not (Variables|/Game/Blueprints/AddOn/Components/BPC_GetHideout.BPC_GetHideout_C|GetIsHidden (Variables|Default|GetBPC_GetHideout)))
    (if (Variables|/Game/Blueprints/AddOn/Components/BPC_GetHideout.BPC_GetHideout_C|GetWantToHideSelf _bpc_gethideout)
      (Default|PlaceSelfinHideout _bpc_gethideout 1.0)))
  (|CallParentFunction DeltaSeconds))

(fn InitState
  (params (Target :type Actor%20Object%20Reference) (StateName :type Byte :default 0) (Commander :type BP%20State%20Commander%20Object%20Reference))
  (|CallParentFunction Target StateName Commander)
  (bind _returnvalue (CallFunction|AddComponent Target))
  (bind _output_get (Variables|Default|SetBPC_GetHideout _returnvalue))
  (Default|Initialize _output_get (Variables|/Game/Blueprints/AI/Pawn/BP_CreatureGeneric.BP_CreatureGeneric_C|GetDetectionArea (Variables|Default|GetSelfCreature)))
  (EventDispatchers|BindEventtoEDonHideoutLeaved _output_get (EventDispatchers|CreateEvent :!event Custom|ED_OnHideoutLeaved_Event))
  (EventDispatchers|BindEventtoEDonHideoutReached _output_get (EventDispatchers|CreateEvent :!event Custom|ED_OnHideoutReached_Event))
  (EventDispatchers|BindEventtoEDonHideoutEnter _output_get (EventDispatchers|CreateEvent :!event Custom|ED_OnHideoutEnter_Event)))

(fn UseSkill
  (bind (_isvalid _returnvalue) (Default|GetNearestHideoutDirection (Variables|Default|GetBPC_GetHideout)))
  (if _isvalid
    (Default|AddDirection (Variables|/Game/Blueprints/AI/Pawn/BP_CreatureGeneric.BP_CreatureGeneric_C|GetBPC_ActorPhysicsMovement (Variables|Default|GetSelfCreature)) _returnvalue))
  (return))

(fn AddComponent
  (params (Target :type Actor%20Object%20Reference))
  (bind _output_get (LocalVariables|SetCurrentBPC (Actor|GetComponentbyClass Target "/Game/Blueprints/AddOn/Components/BPC_GetHideout.BPC_GetHideout_C")))
  (Utilities|IsValid _output_get
    (:Is%20Valid
      _)
    (:Is%20Not%20Valid
      (bind _returnvalue (Game|AddComponentbyClass Target "/Game/Blueprints/AddOn/Components/BPC_GetHideout.BPC_GetHideout_C"))
      (LocalVariables|SetCurrentBPC _returnvalue)))
  (return (LocalVariables|GetCurrentBPC)))