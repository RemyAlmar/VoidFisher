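; Base AI state machine behavior for predator creatures that use a skill, switching movement between hunting and neutral.
; On init it binds to the creature's BPC_Predator prey and hunt events.
; Gaining prey applies Hunter rotation rate and speed from AI data; having none restores Neutre values.
; Hunt and no-prey events set skill usability from prey within range, while prey removal and the skill-available tick do nothing.
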(event Custom|BPC_Predator_ED_HaveToHunt_Event
  (CallFunction|SetCanUseSkill (Default|HasPreyNear (Variables|/Game/Blueprints/AI/Pawn/BP_CreatureGeneric.BP_CreatureGeneric_C|GetBPC_Predator (Variables|Default|GetSelfCreature)) (CallFunction|GetRangeDistance))))

(event Custom|BPC_Predator_ED_OnAddPrey_Event
  (params (PreyToHunt :type Actor%20Object%20Reference))
  (CallFunction|SetRotationRateandSpeed))

(event Custom|BPC_Predator_ED_OnRemovePrey_Event
  (params (PreyToRemoveFromHunt :type Actor%20Object%20Reference)))

(event Custom|BPC_Predator_WithoutPrey_Event
  (CallFunction|SetNeutralRotationRateandSpeed)
  (CallFunction|SetCanUseSkill (Default|HasPreyNear (Variables|/Game/Blueprints/AI/Pawn/BP_CreatureGeneric.BP_CreatureGeneric_C|GetBPC_Predator (Variables|Default|GetSelfCreature)) (CallFunction|GetRangeDistance))))

(event EventWhileSkillAvailableEvent)

(fn InitState
  (params (Target :type Actor%20Object%20Reference) (StateName :type Byte :default 0) (Commander :type BP%20State%20Commander%20Object%20Reference))
  (bind _selfcreature (Variables|Default|GetSelfCreature))
  (bind _bpc_predator (Variables|/Game/Blueprints/AI/Pawn/BP_CreatureGeneric.BP_CreatureGeneric_C|GetBPC_Predator _selfcreature))
  (|CallParentFunction Target StateName Commander)
  (EventDispatchers|BindEventtoEDAddPreytoHunt _bpc_predator (EventDispatchers|CreateEvent :!event Custom|BPC_Predator_ED_OnAddPrey_Event))
  (EventDispatchers|BindEventtoEDHavetoHunt _bpc_predator (EventDispatchers|CreateEvent :!event Custom|BPC_Predator_ED_HaveToHunt_Event))
  (EventDispatchers|BindEventtoEDRemovePreytoHunt _bpc_predator (EventDispatchers|CreateEvent :!event Custom|BPC_Predator_ED_OnRemovePrey_Event))
  (EventDispatchers|BindEventtoEDIsWithoutPrey _bpc_predator (EventDispatchers|CreateEvent :!event Custom|BPC_Predator_WithoutPrey_Event)))

(fn SetNeutralRotationRateandSpeed
  (bind _selfcreature (Variables|Default|GetSelfCreature))
  (bind _value (Default|GetAIData _selfcreature))
  (bind _bpc_actorphysicsmovement (Variables|/Game/Blueprints/AI/Pawn/BP_CreatureGeneric.BP_CreatureGeneric_C|GetBPC_ActorPhysicsMovement _selfcreature))
  (bind (_rotationratedegs _speedms) (Utilities|Struct|BreakS_AICreatureBehaviorSettings _value))
  (Variables|/Game/Blueprints/AddOn/Components/BPC_ActorPhysicsMovement.BPC_ActorPhysicsMovement_C|SetRotationRate _bpc_actorphysicsmovement (.neutre _rotationratedegs))
  (Variables|/Game/Blueprints/AddOn/Components/BPC_ActorPhysicsMovement.BPC_ActorPhysicsMovement_C|SetTargetSpeed _bpc_actorphysicsmovement (.neutre _speedms))
  (return))

(fn SetRotationRateandSpeed
  (bind _selfcreature (Variables|Default|GetSelfCreature))
  (bind _value (Default|GetAIData _selfcreature))
  (bind _bpc_actorphysicsmovement (Variables|/Game/Blueprints/AI/Pawn/BP_CreatureGeneric.BP_CreatureGeneric_C|GetBPC_ActorPhysicsMovement _selfcreature))
  (bind (_rotationratedegs _speedms) (Utilities|Struct|BreakS_AICreatureBehaviorSettings _value))
  (Variables|/Game/Blueprints/AddOn/Components/BPC_ActorPhysicsMovement.BPC_ActorPhysicsMovement_C|SetRotationRate _bpc_actorphysicsmovement (.hunter _rotationratedegs))
  (Variables|/Game/Blueprints/AddOn/Components/BPC_ActorPhysicsMovement.BPC_ActorPhysicsMovement_C|SetTargetSpeed _bpc_actorphysicsmovement (.hunter _speedms)))