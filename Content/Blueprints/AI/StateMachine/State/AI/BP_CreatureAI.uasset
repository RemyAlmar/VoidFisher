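; Base AI state for creatures in the state machine, giving access to the owning BP_CreatureGeneric.
; InitState runs the parent init, caches the cast creature, and binds to its on/off dispatcher and the activate/deactivate dispatchers of its detection, movement and skills state manager components.
; The event handlers, start and quit are empty stubs; update only stores delta time.
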(event Custom|Creature_OnOFFAllBehaviors_Event
  (params (Active :type Boolean)))

(event Custom|ED_MovementManagerOn_Event)

(event Custom|ED_SkillManagerOff_Event)

(event Custom|ED_DetectionManagerOn_Event)

(event Custom|ED_DetectionManagerOff_Event)

(event Custom|ED_SkillManagerOn_Event)

(event Custom|ED_MovementManagerOff_Event)

(event EventIStart)

(event EventIUpdate
  (params (DeltaSeconds :type Float%20%28double-precision%29))
  (Variables|Default|SetDeltaTime DeltaSeconds))

(event EventIQuit)

(fn InitState
  (params (Target :type Actor%20Object%20Reference) (StateName :type Byte :default 0) (Commander :type BP%20State%20Commander%20Object%20Reference))
  (|CallParentFunction Target StateName Commander)
  (bind _target (Variables|Default|GetTarget)
    (:then
      (bind _asbp_creature_generic (Utilities|Casting|CastToBP_CreatureGeneric _target))
      (bind _output_get (Variables|Default|SetSelfCreature _asbp_creature_generic))
      (EventDispatchers|BindEventtoEDON/OFFActivate _output_get (EventDispatchers|CreateEvent :!event Custom|Creature_OnOFFAllBehaviors_Event))
      (EventDispatchers|BindEventtoEDonComponentActivated (Variables|/Game/Blueprints/AI/Pawn/BP_CreatureGeneric.BP_CreatureGeneric_C|GetBPC_StateManager_Detection (Variables|Default|GetSelfCreature)) (EventDispatchers|CreateEvent :!event Custom|ED_DetectionManagerOn_Event))
      (EventDispatchers|BindEventtoEDonComponentDeactivated (Variables|/Game/Blueprints/AI/Pawn/BP_CreatureGeneric.BP_CreatureGeneric_C|GetBPC_StateManager_Detection (Variables|Default|GetSelfCreature)) (EventDispatchers|CreateEvent :!event Custom|ED_DetectionManagerOff_Event))
      (EventDispatchers|BindEventtoEDonComponentActivated (Variables|/Game/Blueprints/AI/Pawn/BP_CreatureGeneric.BP_CreatureGeneric_C|GetBPC_StateManager_Movement (Variables|Default|GetSelfCreature)) (EventDispatchers|CreateEvent :!event Custom|ED_MovementManagerOn_Event))
      (EventDispatchers|BindEventtoEDonComponentDeactivated (Variables|/Game/Blueprints/AI/Pawn/BP_CreatureGeneric.BP_CreatureGeneric_C|GetBPC_StateManager_Movement (Variables|Default|GetSelfCreature)) (EventDispatchers|CreateEvent :!event Custom|ED_MovementManagerOff_Event))
      (EventDispatchers|BindEventtoEDonComponentActivated (Variables|/Game/Blueprints/AI/Pawn/BP_CreatureGeneric.BP_CreatureGeneric_C|GetBPC_StateManager_Skills (Variables|Default|GetSelfCreature)) (EventDispatchers|CreateEvent :!event Custom|ED_SkillManagerOn_Event))
      (EventDispatchers|BindEventtoEDonComponentDeactivated (Variables|/Game/Blueprints/AI/Pawn/BP_CreatureGeneric.BP_CreatureGeneric_C|GetBPC_StateManager_Skills (Variables|Default|GetSelfCreature)) (EventDispatchers|CreateEvent :!event Custom|ED_SkillManagerOff_Event)))
    (:else)))