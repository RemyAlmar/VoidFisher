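; AI state-machine behavior that drives a creature's dash through its BPC_Dash component, running a nested state machine.
; On init it disables the component's tick and binds to its init event, which applies the max cooldown to one state entry and initializes the dash's StateCommander.
; Its update ticks that commander manually.
; The prey's predator-sighting event sets whether dashing is allowed, based on a predator being within range.
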(event Custom|Dash_ED_OnInit_Event
  (bind _list_states_class (Variables|Default|GetList%20States%20Class))
  (bind _value (Utilities|Map|Find _list_states_class 2))
  (bind (_state _distancenormalized) (Utilities|Struct|BreakS_StateCooldown _value))
  (Utilities|Map|Add _list_states_class 2 (Utilities|Struct|MakeS_StateCooldown _state (Variables|Default|GetCooldownMax) _distancenormalized))
  (Default|InititalizeCommander (Variables|/Game/Blueprints/AddOn/Components/BPC_Dash.BPC_Dash_C|GetStateCommander (Variables|Default|GetBPC_Dash)) (Variables|Default|GetSelfCreature) (Variables|Default|GetList%20States%20Class)))

(event EventBPCPreyEDSeePredatorinRange
  (params (TargetPredator :type Actor%20Object%20Reference))
  (Default|SetCanDash (Variables|Default|GetBPC_Dash) (Default|HasPredatorNear (Variables|/Game/Blueprints/AI/Pawn/BP_CreatureGeneric.BP_CreatureGeneric_C|GetBPC_Prey (Variables|Default|GetSelfCreature)) (CallFunction|GetRangeDistance))))

(event EventIUpdate
  (params (DeltaSeconds :type Float%20%28double-precision%29))
  (Default|IUpdate (Variables|/Game/Blueprints/AddOn/Components/BPC_Dash.BPC_Dash_C|GetStateCommander (Variables|Default|GetBPC_Dash)) DeltaSeconds)
  (|CallParentFunction DeltaSeconds))

(fn InitState
  (params (Target :type Actor%20Object%20Reference) (StateName :type Byte :default 0) (Commander :type BP%20State%20Commander%20Object%20Reference))
  (|CallParentFunction Target StateName Commander)
  (bind _asbpc_dash (Utilities|Casting|CastToBPC_Dash (CallFunction|GetComponentInstance (Variables|Default|GetSelfCreature) "/Game/Blueprints/AddOn/Components/BPC_Dash.BPC_Dash_C")))
  (bind _output_get (Variables|Default|SetBPC_Dash _asbpc_dash))
  (Components|Tick|SetComponentTickEnabled _output_get false)
  (EventDispatchers|BindEventtoEDonInit _output_get (EventDispatchers|CreateEvent :!event Custom|Dash_ED_OnInit_Event)))