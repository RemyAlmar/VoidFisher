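; BP_LoadDash is an AI state-machine state that prepares a prey creature's dash and hands over to the dash-use state.
; InitState caches the target's BPC_Dash component, and the predator-in-range event sets skill availability from whether a predator is within range.
; On cooldown reset it clears CanDash and has the Commander switch to the next state, wrapping around the list.
; Other prey reactions are overridden as no-ops.
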(event EventBPCPreyEDonAfraidEvent)

(event EventBPCPreyEDonAimedEvent)

(event EventEDonCooldownResetEvent
  (Default|SetCanDash (Variables|Default|GetBPC_Dash) false)
  (Default|IChangeState (Variables|Default|GetCommander) (Class|KismetMathLibrary|PercentByteByte (+ (Variables|Default|GetEStateName) 1) (Math|Conversions|ToByte(Integer) (Utilities|Map|Length (Variables|/Game/Blueprints/AI/StateMachine/BP_StateCommander.BP_StateCommander_C|GetListStates (Variables|Default|GetCommander))))))
  (|CallParentFunction))

(event EventBPCPreyEDonWithoutPredatorEvent)

(event EventBPCPreyEDReactonPredatorin
  (params (TargetPredator :type Actor%20Object%20Reference)))

(event EventBPCPreyEDReactonPredatorOut
  (params (TargetPredator :type Actor%20Object%20Reference)))

(event EventBPCPreyEDSeePredatorinRange
  (params (TargetPredator :type Actor%20Object%20Reference))
  (CallFunction|SetCanUseSkill (Default|HasPredatorNear (Variables|/Game/Blueprints/AI/Pawn/BP_CreatureGeneric.BP_CreatureGeneric_C|GetBPC_Prey (Variables|Default|GetSelfCreature)) (CallFunction|GetRangeDistance))))

(fn InitState
  (params (Target :type Actor%20Object%20Reference) (StateName :type Byte :default 0) (Commander :type BP%20State%20Commander%20Object%20Reference))
  (|CallParentFunction Target StateName Commander)
  (bind _asbpc_dash (Utilities|Casting|CastToBPC_Dash (CallFunction|TryGetComponent (Variables|Default|GetTarget) "/Game/Blueprints/AddOn/Components/BPC_Dash.BPC_Dash_C")))
  (Variables|Default|SetBPC_Dash _asbpc_dash))