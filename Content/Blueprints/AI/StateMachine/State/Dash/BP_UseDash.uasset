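; Dash skill state for the state machine, usable by AI and input, driven by the owner's BPC_Dash component.
; On start or on the component's dash event, it sets the dash force if active, spawns attached Niagara FX and plays sound.
; Cooldown updates apply the force; cooldown reset re-enables the skill and advances the Commander to the next state, wrapping around.
; The parent UseSkill runs only when a dash sound is valid.
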(event Custom|ED_BPC_Dash_OnUseDashHandle_Event
  (if (Default|IsinCurrentState (Variables|Default|GetCommander) (Variables|Default|GetEStateName))
    (Default|SetDashForce (Variables|Default|GetBPC_Dash))
    (CallFunction|UseSkill)))

(event EventEDonCooldownUpdateEvent
  (params (DeltaTime :type Float%20%28double-precision%29))
  (|CallParentFunction DeltaTime)
  (Default|ApplyDashForce (Variables|Default|GetBPC_Dash)))

(event EventIStart
  (|CallParentFunction)
  (CallFunction|SetSkillAvailable false) ; Force à devoir utiliser can use uniquement (Utile pour IA)
  (if (not (Variables|/Game/Blueprints/AddOn/Components/BPC_Dash.BPC_Dash_C|GetCanDash (Variables|Default|GetBPC_Dash)))
    (CallFunction|EDBPCDashonUseDashHandleEvent)))

(event EventEDonCooldownResetEvent
  (Default|IChangeState (Variables|Default|GetCommander) (Class|KismetMathLibrary|PercentByteByte (+ (Variables|Default|GetEStateName) 1) (Math|Conversions|ToByte(Integer) (Utilities|Map|Length (Variables|/Game/Blueprints/AI/StateMachine/BP_StateCommander.BP_StateCommander_C|GetListStates (Variables|Default|GetCommander))))))
  (CallFunction|SetCanUseSkill true)
  (|CallParentFunction))

(fn InitState
  (params (Target :type Actor%20Object%20Reference) (StateName :type Byte :default 0) (Commander :type BP%20State%20Commander%20Object%20Reference))
  (|CallParentFunction Target StateName Commander)
  (bind _asbpc_dash (Utilities|Casting|CastToBPC_Dash (CallFunction|TryGetComponent (Variables|Default|GetTarget) "/Game/Blueprints/AddOn/Components/BPC_Dash.BPC_Dash_C")))
  (bind _output_get (Variables|Default|SetBPC_Dash _asbpc_dash))
  (EventDispatchers|BindEventtoEDUseDashHandle _output_get (EventDispatchers|CreateEvent :!event Custom|ED_BPC_Dash_OnUseDashHandle_Event)) ; Utile pour Input
)

(fn UseSkill
  (bind _bpc_dash (Variables|Default|GetBPC_Dash))
  (Default|SetCanDash _bpc_dash false)
  (bind _skeletalmesh (Class|BPIGetData|GetSkeletalMesh(Message) (Components|GetOwner _bpc_dash)))
  (Niagara|SpawnSystemAttached (Variables|/Game/Blueprints/AddOn/Components/BPC_Dash.BPC_Dash_C|GetNS_Dash _bpc_dash) (Utilities|ResolveSoftReference _skeletalmesh) "None" "0, 0, 0" "0, 0, 0" "KeepRelativeOffset" true true "AutoRelease")
  (bind _sounddash (Variables|/Game/Blueprints/AddOn/Components/BPC_Dash.BPC_Dash_C|GetSoundDash (Variables|Default|GetBPC_Dash))
    (:then
      (Audio|Components|Audio|Play _sounddash 0.0)
      (|CallParentFunction))
    (:else)))

(fn GetSkeletalMesh
  (return 0))