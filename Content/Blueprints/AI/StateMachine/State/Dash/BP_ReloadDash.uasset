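; BP_ReloadDash is the reload state of the dash skill in the state machine, covering the cooldown after a dash.
; On start it marks the skill unavailable and relies on the parent state's cooldown, clearing IsInDash on the target's BPC_Dash when that cooldown starts.
; When the cooldown resets, it re-enables dashing and tells the Commander to switch to the next state, wrapping around the state list.
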(event EventEDonCooldownResetEvent
  (Default|SetCanDash (Variables|Default|GetBPC_Dash) true)
  (Default|IChangeState (Variables|Default|GetCommander) (Class|KismetMathLibrary|PercentByteByte (+ (Variables|Default|GetEStateName) 1) (Math|Conversions|ToByte(Integer) (Utilities|Map|Length (Variables|/Game/Blueprints/AI/StateMachine/BP_StateCommander.BP_StateCommander_C|GetListStates (Variables|Default|GetCommander))))))
  (|CallParentFunction))

(event EventEDonCooldownUpdateEvent
  (params (DeltaTime :type Float%20%28double-precision%29))
  (|CallParentFunction DeltaTime))

(event EventIStart
  (|CallParentFunction)
  (CallFunction|SetSkillAvailable false)
  (CallFunction|SetCanUseSkill false))

(event EventEDonCooldownStartEvent
  (|CallParentFunction)
  (Variables|/Game/Blueprints/AddOn/Components/BPC_Dash.BPC_Dash_C|SetIsInDash (Variables|Default|GetBPC_Dash) false))

(fn InitState
  (params (Target :type Actor%20Object%20Reference) (StateName :type Byte :default 0) (Commander :type BP%20State%20Commander%20Object%20Reference))
  (|CallParentFunction Target StateName Commander)
  (bind _asbpc_dash (Utilities|Casting|CastToBPC_Dash (CallFunction|TryGetComponent (Variables|Default|GetTarget) "/Game/Blueprints/AddOn/Components/BPC_Dash.BPC_Dash_C")))
  (Variables|Default|SetBPC_Dash _asbpc_dash))