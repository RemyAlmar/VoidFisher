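; Test fish creature that can be caught, which destroys it, and that tracks larger hunters to flee from.
; FleeDetection overlaps add BPI_Hunteable actors whose reported size exceeds its SizeType, and remove them on exit.
; IHaveToFlee reports whether any threats remain, and IFleeing returns the averaged unit direction toward them.
; BeginPlay fires a persistent debug cone of traces to test direction finding, with the result unused.
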(event OnComponentBeginOverlap(FleeDetection)
  (params (OverlappedComponent :type Primitive%20Component%20Object%20Reference) (OtherActor :type Actor%20Object%20Reference) (OtherComp :type Primitive%20Component%20Object%20Reference) (OtherBodyIndex :type Integer) (bFromSweep :type Boolean) (SweepResult :type Hit%20Result%20Structure%20%28by%20ref%29))
  (if (Utilities|DoesObjectImplementInterface OtherActor "/Game/Blueprints/AddOn/Interface/BPI_Hunteable.BPI_Hunteable_C")
    (bind _size (Class|BPIHunteable|IGetSize(Message) OtherActor))
    (bind _isfleeing (CallFunction|IHunted _size))
    (if _isfleeing
      (Utilities|Array|Add (Variables|Default|GetActorToFlee) OtherActor))))

(event OnComponentEndOverlap(FleeDetection)
  (params (OverlappedComponent :type Primitive%20Component%20Object%20Reference) (OtherActor :type Actor%20Object%20Reference) (OtherComp :type Primitive%20Component%20Object%20Reference) (OtherBodyIndex :type Integer))
  (if (Utilities|Array|ContainsItem (Variables|Default|GetActorToFlee) OtherActor)
    (Utilities|Array|RemoveItem (Variables|Default|GetActorToFlee) OtherActor)))

(event EventCatched
  (Actor|DestroyActor))

(event EventBeginPlay
  (CallFunction|GetOneDirectionfromFirstConeHit 8 (Transformation|GetActorLocation) (Transformation|GetActorForwardVector) 6e+01 1e+03 "TraceTypeQuery1" "Persistent" 0.0 "(R=1.000000,G=0.000000,B=0.118750,A=1.000000)"))

(fn ConstructionScript)

(fn InitializeUniqueData
  (params (UserData :type S%20Catcheable%20Data%20Structure))
  (Variables|Data|SetUserData UserData))

(fn GetData
  (return "NewEnumerator3" (Variables|Data|GetUserData)))

(fn IFleeing
  (for _array_element (Variables|Default|GetActorToFlee)
    (LocalVariables|SetMedianVector (+ (LocalVariables|GetMedianVector) (Math|Vector|GetUnitDirection(Vector) (Transformation|GetActorLocation) (Transformation|GetActorLocation _array_element)))))
  (bind _output_get (LocalVariables|SetMedianVector (/ (LocalVariables|GetMedianVector) (Utilities|Array|Length (Variables|Default|GetActorToFlee)))))
  (return _output_get))

(fn IGetSize
  (return 0))

(fn IHavetoFlee
  (return (Utilities|Array|IsNotEmpty (Variables|Default|GetActorToFlee))))

(fn IHunted
  (params (Byte :type Byte :default 0))
  (bind _data (CallFunction|GetData))
  (return (< (Math|Conversions|ToInteger(Byte) (.sizetype _data)) Byte)))

(fn IsCatcheable
  (return true))