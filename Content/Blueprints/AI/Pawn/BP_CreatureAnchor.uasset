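; BP_CreatureAnchor is a creature pawn variant that carries anchors and cannot be caught while any anchor is active.
; On initialization it collects the skeletal mesh sockets whose names contain "Anchor" and passes them to BPCAnchorManager, with the creature's size stat as anchor radius.
; Activation runs the parent logic, then forwards the state to the anchor manager.
; The catchable check queries that manager for active anchors.
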(fn ConstructionScript
  (|CallParentFunction))

(fn GetSocketName
  (params (TargetName :type String))
  (for _array_element (Transformation|GetAllSocketNames (Variables|Default|GetSKM_Creature))
    (if (Utilities|String|Contains (Utilities|String|ToString(Name) _array_element) TargetName)
      (Utilities|Array|Add (LocalVariables|GetSocketAnchorList) _array_element)))
  (return (LocalVariables|GetSocketAnchorList)))

(fn Initialize
  (params (CreatureDetails :type S%20Creature%20Details%20Structure))
  (|CallParentFunction CreatureDetails)
  (Default|Initialize (Variables|Default|GetBPC_AnchorManager) false (Variables|Default|GetSKM_Creature) (.Size (Utilities|Struct|BreakS_AICreatureStatSettings (Utilities|Struct|BreakS_CreatureDetailsInstanced (Variables|Default|GetUserData)))) (CallFunction|GetSocketName "Anchor")))

(fn Activate
  (params (Active :type Boolean))
  (|CallParentFunction Active)
  (Default|OnComponentActivate (Variables|Default|GetBPC_AnchorManager) Active))

(fn IIsCatcheable
  (return (not (.HasAnyAnchorActive (Default|HasAnchorActive (Variables|Default|GetBPC_AnchorManager))))))