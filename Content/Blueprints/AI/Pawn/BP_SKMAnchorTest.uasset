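; BP_SKMAnchorTest is an AI pawn Blueprint that sets up anchors on a skeletal mesh creature, apparently as a test.
; On BeginPlay it gathers every socket on SKMCreature whose name contains "Anchor".
; It initializes BPCAnchorManager with that socket list, the mesh as parent, and the mesh's largest world-scale axis as the anchor radius.
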(event EventBeginPlay
  (Default|Initialize (Variables|Default|GetBPC_AnchorManager) false (Variables|Default|GetSKM_Creature) (Math|Vector|GetMaxElement (Transformation|GetWorldScale (Variables|Default|GetSKM_Creature))) (CallFunction|GetSocketName "Anchor")))

(fn ConstructionScript)

(fn GetSocketName
  (params (TargetName :type String))
  (for _array_element (Transformation|GetAllSocketNames (Variables|Default|GetSKM_Creature))
    (if (Utilities|String|Contains (Utilities|String|ToString(Name) _array_element) TargetName)
      (Utilities|Array|Add (LocalVariables|GetSocketAnchorList) _array_element)))
  (return (LocalVariables|GetSocketAnchorList)))