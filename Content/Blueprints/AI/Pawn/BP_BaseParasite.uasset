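; BP_BaseParasite is a parasite base that handles its own Niagara visuals and dissolve-out death.
; BeginPlay spawns and stores the base effect at the actor's transform, while SpawnFlaque spawns a separate pop effect there.
; Dissolve sets the effect's Despawn flag to false and drives its Dissolve parameter through a timeline.
; When the timeline finishes, it destroys the effect and actor, then requests an attached death-zone sound.
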(event Custom|Spawn%20Flaque
  (bind _returnvalue (Transformation|GetActorTransform))
  (Niagara|SpawnSystematLocation "/Game/VFX/Niagara/Parasite/NS_ParasitePop.NS_ParasitePop" (.location _returnvalue) (.rotation _returnvalue)))

(event Custom|Dissolve
  (bind _ns_baseparasite (Variables|Default|GetNS_BaseParasite))
  (Class|NiagaraComponent|SetVariableBool _ns_baseparasite "Despawn" false)
  (bind _alpha (Timeline|Alpha PlayFromStart)
    (:Update
      (Niagara|SetNiagaraVariable(Float) _ns_baseparasite "Dissolve" _alpha))
    (:Finished
      (Components|DestroyComponent _ns_baseparasite)
      (Actor|DestroyActor)
      (Audio|SpawnSoundAttached "/Game/SFX/Sounds/PLACEHOLDER/ParasyteZoneDeath_Cue.ParasyteZoneDeath_Cue" (Variables|Default|GetBaseParasite) "None" "0, 0, 0" "0, 0, 0" "KeepRelativeOffset" true 1.0 1.0 0.0 "/Game/SFX/Sounds/PLACEHOLDER/Attenuation/SFX_ATT_ParasyteDeadZone.SFX_ATT_ParasyteDeadZone" 0 false))))

(event EventBeginPlay
  (bind _returnvalue (Transformation|GetActorTransform))
  (bind _returnvalue_2 (Niagara|SpawnSystematLocation "/Game/VFX/Niagara/Parasite/NS_BaseParasite.NS_BaseParasite" (.location _returnvalue) (.rotation _returnvalue) "1.000000,1.000000,1.000000" false))
  (Variables|Default|SetNS_BaseParasite _returnvalue_2))

(fn ConstructionScript)