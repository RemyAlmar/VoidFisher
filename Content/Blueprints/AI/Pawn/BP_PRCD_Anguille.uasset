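; Procedural eel AI pawn whose body trails its head in a sinuous swimming motion.
; Construction builds a world-detached chain of mesh instances, spans it with body and tail spline meshes, tapers their scale and sizes the head.
; Each tick, the first instance snaps to the actor and the others lerp toward their predecessor, offset by a sine wave that grows along the body.
; The spline meshes then copy the instances' positions, tangents and roll.
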(event EventTick
  (params (DeltaSeconds :type Float%20%28single-precision%29))
  (|CallParentFunction DeltaSeconds)
  (CallFunction|SnakeMovement DeltaSeconds)
  (CallFunction|UpdateSpline))

(fn ConstructionScript
  (bind _ism_tail (Variables|Default|GetISM_Tail))
  (bind _instance_transform_scale (Variables|Public|Snake|Transform|GetInstance%20Transform%20Scale))
  (bind _ism_tail_2 (Variables|Default|GetISM_Tail))
  (|CallParentFunction)
  (Components|InstancedStaticMesh|ClearInstances _ism_tail)
  (Transformation|DetachFromComponent _ism_tail "KeepWorld" "KeepWorld" "KeepWorld" true)
  (for _index (range 0 (Variables|Public|Snake|GetLength))
    (Components|InstancedStaticMesh|AddInstance _ism_tail_2 (Math|Transform|MakeTransform (Math|Vector|MakeVector (Math|Conversions|ToFloat(Integer) (* (* _index (Variables|Public|Snake|Transform|GetSpacing)) _instance_transform_scale)) 0.0 0.0) "0, 0, 0" (* "1.000000,1.000000,1.000000" _instance_transform_scale)) false)
    (if (== _index (Variables|Public|Snake|GetLength))
      (Components|StaticMesh|SetStaticMesh _ism_tail_2 (Variables|Public|Snake|GetTailMesh))
      (else
        (Components|StaticMesh|SetStaticMesh _ism_tail_2 (.OutItem (Utilities|Array|Random (Variables|Public|Snake|GetBodyMesh)))))))
  (CallFunction|SetSplineMesh)
  (CallFunction|SetSplineScale)
  (Transformation|SetWorldScale3D (Variables|Default|GetSKM_Creature) (* "1.000000,1.000000,1.000000" (Variables|Public|Snake|Transform|GetHead%20Scale))))

(fn SetSplineMesh
  (bind _ism_tail (Variables|Default|GetISM_Tail))
  (bind _returnvalue (Components|InstancedStaticMesh|GetInstanceCount _ism_tail))
  (bind _returnvalue_2 (- _returnvalue 1))
  (for _index (range 0 _returnvalue_2)
    (bind _returnvalue_3 (AddComponent|AddSplineMeshComponent true))
    (LocalVariables|SetSplineMesh _returnvalue_3)
    (if (== _index _returnvalue_2)
      (Components|StaticMesh|SetStaticMesh (LocalVariables|GetSplineMesh) (Variables|Public|Snake|GetTailMesh))
      (else
        (Components|StaticMesh|SetStaticMesh (LocalVariables|GetSplineMesh) (.OutItem (Utilities|Array|Random (Variables|Public|Snake|GetBodyMesh))))))
    ;[0.3666 1 0.6168] Start
    (SplineMesh|SetStartPosition (LocalVariables|GetSplineMesh) (.location (.OutInstanceTransform (Components|InstancedStaticMesh|GetInstanceTransform _ism_tail (+ _index 1) true))) true)
    (SplineMesh|SetStartTangent (LocalVariables|GetSplineMesh) (Math|Vector|GetForwardVector (.rotation (.OutInstanceTransform (Components|InstancedStaticMesh|GetInstanceTransform _ism_tail (+ _index 1) true)))) true :!class /Script/Engine.SplineMeshComponent)
    ;[0.7344 0.4688 1] End
    (SplineMesh|SetEndPosition (LocalVariables|GetSplineMesh) (.location (.OutInstanceTransform (Components|InstancedStaticMesh|GetInstanceTransform _ism_tail _index true))) true)
    (SplineMesh|SetEndTangent (LocalVariables|GetSplineMesh) (Math|Vector|GetForwardVector (.rotation (.OutInstanceTransform (Components|InstancedStaticMesh|GetInstanceTransform _ism_tail _index true)))) true :!class /Script/Engine.SplineMeshComponent)
    (Utilities|Array|Add (Variables|Private|Transform|GetSplineMeshComponent) (LocalVariables|GetSplineMesh))))

(fn UpdateSpline
  (bind _ism_tail (Variables|Default|GetISM_Tail))
  (for (_array_element _array_index) (Variables|Private|Transform|GetSplineMeshComponent)
    ;[0.3666 1 0.6168] Start
    (SplineMesh|SetStartPosition _array_element (.location (.OutInstanceTransform (Components|InstancedStaticMesh|GetInstanceTransform _ism_tail (+ _array_index 1) true))) true)
    (SplineMesh|SetStartTangent _array_element (Math|Vector|GetForwardVector (.rotation (.OutInstanceTransform (Components|InstancedStaticMesh|GetInstanceTransform _ism_tail (+ _array_index 1) true)))) true :!class /Script/Engine.SplineMeshComponent)
    ;[0.7344 0.4688 1] End
    (SplineMesh|SetEndPosition _array_element (.location (.OutInstanceTransform (Components|InstancedStaticMesh|GetInstanceTransform _ism_tail _array_index true))) true)
    (SplineMesh|SetEndTangent _array_element (Math|Vector|GetForwardVector (.rotation (.OutInstanceTransform (Components|InstancedStaticMesh|GetInstanceTransform _ism_tail _array_index true)))) true :!class /Script/Engine.SplineMeshComponent)
    ;[1 0.8139 0.481] Rotation
    (SplineMesh|SetStartRollDegrees _array_element (.Roll (Math|Rotator|BreakRotator (.rotation (.OutInstanceTransform (Components|InstancedStaticMesh|GetInstanceTransform _ism_tail (+ _array_index 1) true))))) true)
    (SplineMesh|SetEndRollDegrees _array_element (.Roll (Math|Rotator|BreakRotator (.rotation (.OutInstanceTransform (Components|InstancedStaticMesh|GetInstanceTransform _ism_tail _array_index true))))) true)))

(fn GetScale
  (params (ID :type Integer))
  (bind _max_scale (Variables|Public|Snake|Transform|GetMax%20Scale))
  (bind _splinemeshcomponent (Variables|Private|Transform|GetSplineMeshComponent))
  (bind _minscale (Variables|Public|Snake|Transform|GetMinScale))
  (bind _spline_scale (Variables|Public|Snake|Transform|GetSpline%20Scale))
  (bind _returnvalue (Utilities|Array|Length _splinemeshcomponent))
  (bind _returnvalue_2 (- _returnvalue ID))
  (bind _returnvalue_3 (/ _returnvalue_2 _returnvalue))
  (bind _returnvalue_4 (* _returnvalue_3 _spline_scale))
  (bind _returnvalue_5 (Math|Float|Clamp(Float) _returnvalue_4 _minscale _max_scale))
  (return (Math|Vector2D|MakeVector2D _returnvalue_5 _returnvalue_5)))

(fn SetSplineScale
  (for _index (range 0 (- (Utilities|Array|Length (Variables|Private|Transform|GetSplineMeshComponent)) 1))
    (bind _output_get (LocalVariables|SetSplineMeshComponent (Utilities|Array|Get(acopy) (Variables|Private|Transform|GetSplineMeshComponent) _index)))
    (SplineMesh|SetStartScale _output_get (CallFunction|GetScale (+ _index 1)) true :!class /Script/Engine.SplineMeshComponent)
    (SplineMesh|SetEndScale _output_get (CallFunction|GetScale _index) true :!class /Script/Engine.SplineMeshComponent)))

(fn SnakeMovement
  (params (Tick :type Float%20%28double-precision%29))
  (bind _returnvalue (Transformation|GetActorTransform))
  (bind _instancetransform (Variables|Private|Transform|GetInstanceTransform))
  (bind _ism_tail (Variables|Default|GetISM_Tail))
  (Utilities|Array|Clear (Variables|Private|Transform|GetInstanceTransform))
  (for _index (range 0 (- (Components|InstancedStaticMesh|GetInstanceCount _ism_tail) 1))
    (Utilities|Array|Add (Variables|Private|Transform|GetInstanceTransform) (.OutInstanceTransform (Components|InstancedStaticMesh|GetInstanceTransform _ism_tail _index true))))
  (Components|InstancedStaticMesh|UpdateInstanceTransform _ism_tail 0 (Math|Transform|MakeTransform (.location _returnvalue) (.rotation _returnvalue) (.scale (Utilities|Array|Get(acopy) (Variables|Private|Transform|GetInstanceTransform)))) true false false) ; Le premier élément
  (for (_array_element _array_index) _instancetransform
    ;[1 0.3294 0.8534] Calcul du sinus
    (LocalVariables|SetOffset%20Y (* (Math|Trig|Sin(Degrees) (+ (* (+ _array_index 1) 25.0) (* (Utilities|Time|GetGameTimeinSeconds) 1e+02))) 1e+03))
    ;[1 0.5978 0.3421] Udate final du world transform
    (Components|InstancedStaticMesh|UpdateInstanceTransform (Variables|Default|GetISM_Tail) (+ _array_index 1) (Math|Transform|Lerp(Transform) (.OutInstanceTransform (Components|InstancedStaticMesh|GetInstanceTransform (Variables|Default|GetISM_Tail) (+ _array_index 1) true)) (Math|Transform|MakeTransform (Math|Vector|MakeVector (+ (.X (Math|Vector|BreakVector (+ (* (Math|Vector|GetRightVector (.Rotation (Math|Transform|BreakTransform _array_element))) (* (LocalVariables|GetOffset%20Y) (Math|Float|NormalizetoRange (+ (Math|Conversions|ToFloat(Integer) _array_index) -1.0) 0.0 (Math|Conversions|ToFloat(Integer) (- (Utilities|Array|Length _instancetransform) 1))))) (* (Math|Vector|GetUpVector (.Rotation (Math|Transform|BreakTransform _array_element))) (* (LocalVariables|GetOffset%20Y) (Math|Float|NormalizetoRange (+ (Math|Conversions|ToFloat(Integer) _array_index) -1.0) 0.0 (Math|Conversions|ToFloat(Integer) (- (Utilities|Array|Length _instancetransform) 1)))))))) (.X (Math|Vector|BreakVector (.Location (Math|Transform|BreakTransform _array_element))))) (+ (.Y (Math|Vector|BreakVector (+ (* (Math|Vector|GetRightVector (.Rotation (Math|Transform|BreakTransform _array_element))) (* (LocalVariables|GetOffset%20Y) (Math|Float|NormalizetoRange (+ (Math|Conversions|ToFloat(Integer) _array_index) -1.0) 0.0 (Math|Conversions|ToFloat(Integer) (- (Utilities|Array|Length _instancetransform) 1))))) (* (Math|Vector|GetUpVector (.Rotation (Math|Transform|BreakTransform _array_element))) (* (LocalVariables|GetOffset%20Y) (Math|Float|NormalizetoRange (+ (Math|Conversions|ToFloat(Integer) _array_index) -1.0) 0.0 (Math|Conversions|ToFloat(Integer) (- (Utilities|Array|Length _instancetransform) 1)))))))) (.Y (Math|Vector|BreakVector (.Location (Math|Transform|BreakTransform _array_element))))) (+ (.Z (Math|Vector|BreakVector (+ (* (Math|Vector|GetRightVector (.Rotation (Math|Transform|BreakTransform _array_element))) (* (LocalVariables|GetOffset%20Y) (Math|Float|NormalizetoRange (+ (Math|Conversions|ToFloat(Integer) _array_index) -1.0) 0.0 (Math|Conversions|ToFloat(Integer) (- (Utilities|Array|Length _instancetransform) 1))))) (* (Math|Vector|GetUpVector (.Rotation (Math|Transform|BreakTransform _array_element))) (* (LocalVariables|GetOffset%20Y) (Math|Float|NormalizetoRange (+ (Math|Conversions|ToFloat(Integer) _array_index) -1.0) 0.0 (Math|Conversions|ToFloat(Integer) (- (Utilities|Array|Length _instancetransform) 1)))))))) (.Z (Math|Vector|BreakVector (.Location (Math|Transform|BreakTransform _array_element)))))) (.Rotation (Math|Transform|BreakTransform _array_element)) (.Scale (Math|Transform|BreakTransform _array_element))) (Variables|Public|Snake|GetSpeed)) true false false) ; Les autres éléments
  ))