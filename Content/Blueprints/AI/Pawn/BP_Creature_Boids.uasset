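; BP_Creature_Boids is an AI creature pawn that represents a fish school, with a Niagara boid system around a lead "mother" fish.
; On Initialize, it feeds creature data into Niagara: quantity, static mesh, size and neutral speed as base attraction strength.
; Each Tick rescales attraction strength by the lead fish's physics-movement speed relative to its neutral speed.
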(event EventTick
  (params (DeltaSeconds :type Float%20%28single-precision%29))
  ;[1 0.6418 0.602] Change Force by Speed
  (|CallParentFunction DeltaSeconds)
  (Niagara|SetNiagaraVariable(Float) (Variables|Default|GetNS_boids) "Attraction Strength001" (* (/ (/ (* (Default|GetSpeed (Variables|Default|GetBPC_ActorPhysicsMovement)) 1e+02) (.neutre (.speedms (.creaturebehaviorsettings (Variables|Default|GetUserData))))) 1e+02) (Variables|Default|GetBoid%20Speed))) ; Set l'attraction Force par rapport à la vitesse du poisson mere
)

(fn ConstructionScript
  (|CallParentFunction))

(fn Initialize
  (params (CreatureDetails :type S%20Creature%20Details%20Structure))
  (bind _ns_boids (Variables|Default|GetNS_boids))
  (bind _userdata (Variables|Default|GetUserData))
  (bind _userdata_2 (Variables|Default|GetUserData))
  (|CallParentFunction CreatureDetails)
  (Class|NiagaraComponent|SetVariableInt _ns_boids "Spawn Count" (.quantity (.creaturestatsettings _userdata)))
  (Class|NiagaraComponent|SetVariableStaticMesh _ns_boids "CreatureMeshs" (.staticmesh (.creaturestatsettings _userdata)))
  (Niagara|SetNiagaraVariable(Float) (Variables|Default|GetNS_boids) "Attraction Strength001" (.neutre (.speedms (.creaturebehaviorsettings _userdata_2))))
  (Variables|Default|SetBoid%20Speed (.neutre (.speedms (.creaturebehaviorsettings _userdata_2))))
  (Niagara|SetNiagaraVariable(Float) (Variables|Default|GetNS_boids) "BoidScaleMesh" (.size (.creaturestatsettings _userdata_2))))