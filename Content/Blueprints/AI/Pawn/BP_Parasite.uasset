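; BP_Parasite is a parasite creature that sticks to surfaces and can be pulled loose with a hook.
; At construction it aligns its skeletal mesh to the root sphere and, with AutoSnap, uses cone traces to snap onto the nearest surface.
; BeginPlay initializes the anchor manager and reveals one of three random static meshes.
; A strong enough pull enables physics, then after a delay calls ICatched and removes the hook.
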(event EDonAttachHook(BPC_AnchorManager))

(event EDonDetachHook(BPC_AnchorManager))

(event EDonHookPulled(BPC_AnchorManager)
  (params (Strength :type Float%20%28double-precision%29) (TensionDirection :type Vector :default "0, 0, 0"))
  (if (>= Strength 1.4e+05)
    (if (not (Physics|IsSimulatingPhysics (Variables|Default|GetRoot) "None"))
      (Default|SetSimulatePhysics (Variables|Default|GetBPC_AnchorManager) true)
      (Utilities|FlowControl|Delay 3.0)
      (CallFunction|ICatched)
      (bind _hookcomp (Variables|/Game/Blueprints/AddOn/Components/BPC_AnchorManager.BPC_AnchorManager_C|GetHookComp (Variables|Default|GetBPC_AnchorManager))
        (:then
          (Default|EDRemoveHookonAnchorEvent _hookcomp))
        (:else)))))

(event EventBeginPlay
  (|CallParentFunction)
  (Default|Initialize (Variables|Default|GetBPC_AnchorManager) true (Variables|Default|GetRoot) 1.0)
  (Development|SetHiddeninGame (.OutItem (Utilities|Array|Random (Utilities|Array|MakeArray (Variables|Default|GetStaticMesh1) (Variables|Default|GetStaticMesh2) (Variables|Default|GetStaticMesh)))) false false))

(fn ConstructionScript
  (|CallParentFunction)
  (Transformation|SetRelativeLocation (Variables|Default|GetSKM_Creature) (Math|Vector|MakeVector 0.0 0.0 (* (Variables|/Script/Engine.SphereComponent|GetSphereRadius (Variables|Default|GetRoot)) -1.0)) false false)
  (if (Variables|Construct|Parameters|GetAutoSnap)
    (Construct|Parameters|SnapQuicklyActoronNearestSurface)))

(fn GetSocketName
  (params (TargetName :type String))
  (for _array_element (Transformation|GetAllSocketNames (Variables|Default|GetSKM_Creature))
    (if (Utilities|String|Contains (Utilities|String|ToString(Name) _array_element) TargetName)
      (Utilities|Array|Add (LocalVariables|GetSocketAnchorList) _array_element)))
  (return (LocalVariables|GetSocketAnchorList)))

(fn SnapQuicklyActoronNearestSurface
  (bind (_nearesthit _hasahit) (CallFunction|GetNearestHitLocationfromSphereRadius (Variables|Construct|Parameters|GetAccuracySnap) (Transformation|GetActorLocation) (Transformation|GetActorUpVector) (Transformation|GetActorRightVector) 1e+01 (Variables|Construct|Parameters|GetRangeSnap) 360 "TraceTypeQuery3" "None" 3.0 "(R=0.000000,G=0.537358,B=1.000000,A=1.000000)"))
  (if _hasahit
    (LocalVariables|SetNextRotation (Math|Rotator|MakeRotfromZ (.Normal (Collision|BreakHitResult _nearesthit))))
    (LocalVariables|SetNextLocation (+ (.Location (Collision|BreakHitResult _nearesthit)) (* (.Normal (Collision|BreakHitResult _nearesthit)) (Variables|/Script/Engine.SphereComponent|GetSphereRadius (Variables|Default|GetRoot)))))
    (Transformation|SetActorRotation (LocalVariables|GetNextRotation))
    (Transformation|SetActorLocation (LocalVariables|GetNextLocation) false false)))