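; BP_CreatureGeneric is the generic AI creature pawn, apparently fish, that detects prey and predators and can be caught.
; Initialize applies data-table details, randomizing size, weight and quantity, then configures mesh, movement, detection sphere and prey/predator components.
; Three state managers (movement, detection, skills) receive per-creature state lists, while sphere traces and cone raycasts provide speed-scaled obstacle avoidance.
; It also handles activation toggling, player-detection feedback, catchable visuals and capture effects before destruction.
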(event EDonStopInvulnerability(BPC_BounceManager)
  ;[1 0.5461 0] Reset la vitesse quand plus invulnerable
  (Default|CallEDResetSpeed))

(event EDReactonPredatorin(BPC_Prey)
  (params (TargetPredator :type Actor%20Object%20Reference))
  ;[0.2492 1 0] Prey Event
  (Utilities|Casting|CastToBP_PlayerRefonte TargetPredator)
  (Niagara|SpawnSystemAttached "/Game/VFX/Niagara/Fish/NS_FishSeeYou.NS_FishSeeYou" (Variables|Default|GetSKM_Creature) "VFX_Socket" "0, 0, 0" (Transformation|GetActorRotation) "SnapToTargetIncludingScale" true)
  (bind _returnvalue (Audio|SpawnSoundatLocation (Utilities|Struct|BreakS_CreatureDetailsInstanced (Variables|Data|GetUserData)) (Transformation|GetActorLocation) "0, 0, 0" 1.0 1.0 0.0 0 0))
  (Variables|Default|SetSoundFish _returnvalue))

(event EDSeePredatorinRange(BPC_Prey)
  (params (TargetPredator :type Actor%20Object%20Reference))
  ;[0.2492 1 0] Prey Event
)

(event EDonAimed(BPC_Prey)
  ;[0.2492 1 0] Prey Event
)

(event EDReactonPredatorOut(BPC_Prey)
  (params (TargetPredator :type Actor%20Object%20Reference))
  ;[0.2492 1 0] Prey Event
)

(event EDonWithoutPredator(BPC_Prey)
  ;[0.2492 1 0] Prey Event
)

(event EDonAfraid(BPC_Prey)
  ;[0.2492 1 0] Prey Event
)

(event Custom|ED_DestroyActor_Event
  ;[0.1264 1 0.2602] Quand la creature est detruite
  (Default|CallEDonDestroyActor self)
  (Utilities|FlowControl|DelayUntilNextTick)
  (Actor|DestroyActor))

(event Custom|BecomeNotCatcheable_Event
  (bind _bpc_vfx_manager (Variables|Default|GetBPC_VFX_Manager))
  ;[0.2492 1 0] Prey Event
  (Default|SetMaterialNiagaraSystem _bpc_vfx_manager "NewEnumerator1" "Material" (Default|GetMaterialNiagaraSystem _bpc_vfx_manager "NewEnumerator1")))

(event Custom|BecomeCatcheable_Event
  ;[0.2492 1 0] Prey Event
  (Default|SetMaterialNiagaraSystem (Variables|Default|GetBPC_VFX_Manager) "NewEnumerator1" "Material" "/Game/VFX/Materials/Fish/M_Net.M_Net"))

(event Custom|ED_OnStunned_Event
  ;[0.2353 0.6926 1] On Stun
  (Default|CallEDonStunned))

(event Custom|ED_ON/OFFActivate_Event
  (params (Active :type Boolean))
  (CallFunction|Activate Active)
  (Default|CallEDON/OFFActivate Active))

(event EventICatched
  (params (Niagara :type Niagara%20System%20Object%20Reference))
  (bind _skm_creature (Variables|Default|GetSKM_Creature))
  (bind _returnvalue (Transformation|GetWorldTransform _skm_creature))
  ;[0.4861 0.8484 1] Catched
  (Niagara|SpawnSystematLocation Niagara (.location _returnvalue) (.rotation _returnvalue) (.scale _returnvalue))
  (bind _soundfish (Variables|Default|GetSoundFish)
    (:then
      (Audio|Components|Audio|Stop _soundfish))
    (:else
      _))
  (Audio|SpawnSound2D "/Game/SFX/Sounds/NEW_OGG/Menu_UI_UX/In_Game/SFX_SpeceFoundAgain_Cue.SFX_SpeceFoundAgain_Cue" 0.9 1.0 0.0 "/Game/SFX/Sounds/PLACEHOLDER/SoundConccurency/SC_Capture.SC_Capture")
  (CallFunction|EDDestroyActorEvent))

(event EventISetMicroArea
  (params (TargetArea :type E_MicroZone%20Enum :default "NewEnumerator4"))
  (Variables|Data|SetCurrentMicroArea TargetArea))

(event EventIHealthed
  ;[0.2492 1 0] Prey Event
  (Default|CallEDonHealthed self))

(fn ConstructionScript)

(fn Initialize
  (params (CreatureDetails :type S%20Creature%20Details%20Structure))
  (bind (_skeletalmesh _animblueprint _staticmesh _material _sizeminmaxm _weightminmaxkg _quantityminmax _xp _niagarasystem) (Utilities|Struct|BreakS_AICreatureRenderSettings (.creaturerendering CreatureDetails)))
  (bind _bpc_informationdata (Variables|Default|GetBPC_InformationData))
  (bind _infos (Default|GetInformations _bpc_informationdata))
  (bind (_primarycolor _secondarycolor) (Utilities|Struct|BreakS_InformationData _infos))
  ;[0.5021 1 0.5631] Initialize all variables from data table
  (Variables|Data|SetUserData (Utilities|Struct|MakeS_CreatureDetailsInstanced (.creaturename CreatureDetails) (.creaturesizetype CreatureDetails) (.creaturedescription CreatureDetails) (Utilities|Struct|MakeS_AICreatureStatSettings _skeletalmesh _animblueprint _staticmesh _material (CallFunction|GetRandomFloatfromVector _sizeminmaxm) (CallFunction|GetRandomFloatfromVector _weightminmaxkg) (CallFunction|GetRandomIntfromVectorInt _quantityminmax) _xp _niagarasystem) (.creaturebehaviorsettings CreatureDetails) (.soundfish CreatureDetails) (.parambystring CreatureDetails)))
  (Default|AddParamsWithoutModify (Variables|Default|GetBPC_ParamsByString) (.ParamByString (Utilities|Struct|BreakS_CreatureDetailsInstanced (Variables|Data|GetUserData))))
  (Render|SetMesh (.CreatureMesh (Utilities|Struct|BreakS_AICreatureStatSettings (.CreatureStatSettings (Utilities|Struct|BreakS_CreatureDetailsInstanced (Variables|Data|GetUserData))))) (.Size (Utilities|Struct|BreakS_AICreatureStatSettings (.CreatureStatSettings (Utilities|Struct|BreakS_CreatureDetailsInstanced (Variables|Data|GetUserData))))))
  (Default|AddNiagaraSystem (Variables|Default|GetBPC_VFX_Manager) "NewEnumerator1" true "0, 0, 0" "0, 0, 0" "1.000000,1.000000,1.000000" true true "Root" "ToolIcon" 0 true)
  (Default|SetFloatNiagaraSystem (Variables|Default|GetBPC_VFX_Manager) "NewEnumerator1" "SpriteSize" (Default|GetValuebyParamName (Variables|Default|GetBPC_ParamsByString) "SpriteSize"))
  (AI|SetBehaviorSettings (.CreatureBehaviorSettings (Utilities|Struct|BreakS_CreatureDetailsInstanced (Variables|Data|GetUserData))) (.Size (Utilities|Struct|BreakS_AICreatureStatSettings (.CreatureStatSettings (Utilities|Struct|BreakS_CreatureDetailsInstanced (Variables|Data|GetUserData))))))
  (Class|SkeletalMeshComponent|SetAnimClass (Variables|Default|GetSKM_Creature) (.AnimBlueprint (Utilities|Struct|BreakS_AICreatureStatSettings (.CreatureStatSettings (Utilities|Struct|BreakS_CreatureDetailsInstanced (Variables|Data|GetUserData))))))
  (AI|Settings|SetandBindComponents)
  (Default|SetInfos _bpc_informationdata (Utilities|Struct|MakeS_InformationData (Utilities|Text|ToText(String) (Utilities|String|EnumtoString (Utilities|Struct|BreakS_CreatureDetailsInstanced (Variables|Data|GetUserData)))) _primarycolor _secondarycolor))
  (Variables|Default|SetNiagara%20System (Utilities|Struct|BreakS_AICreatureStatSettings (Utilities|Struct|BreakS_CreatureDetailsInstanced (Variables|Data|GetUserData)))))

(fn GetAIData
  (return (.creaturebehaviorsettings (Variables|Data|GetUserData))))

(fn SetDetectionRange
  (params (DetectionRange :type Vector%202D%20Structure))
  (Components|Sphere|SetSphereRadius (Variables|Default|GetDetectionArea) (.x DetectionRange) true)
  (return))

(fn SetBehaviorSettings
  (params (BehaviorSettings :type S%20AI%20Creature%20Behavior%20Settings%20Structure%20%28by%20ref%29) (SizeToScale :type Float%20%28double-precision%29))
  (bind (_hunter _prey _neutre) (Utilities|Struct|BreakS_FloatCreatureMode (.rotationratedegs BehaviorSettings)))
  (bind (_hunter_2 _prey_2 _neutre_2) (Utilities|Struct|BreakS_FloatCreatureMode (.speedms BehaviorSettings)))
  (bind _root (Variables|Default|GetRoot))
  (bind _creaturestateslist (Utilities|Struct|BreakS_AICreatureBehaviorSettings BehaviorSettings))
  (bind (_detectmovementlist _detectstatelist _skillstatelist) (Utilities|Struct|BreakS_AICreatureStates _creaturestateslist))
  (Variables|/Game/Blueprints/AddOn/Components/BPC_ActorPhysicsMovement.BPC_ActorPhysicsMovement_C|SetMaxRotationRate (Variables|Default|GetBPC_ActorPhysicsMovement) (Math|Vector|GetMaxElement (Math|Vector|MakeVector _hunter _prey _neutre)))
  (Variables|Default|SetTargetTempSpeed _neutre_2)
  (Variables|/Game/Blueprints/AddOn/Components/BPC_ActorPhysicsMovement.BPC_ActorPhysicsMovement_C|SetMaxSpeed (Variables|Default|GetBPC_ActorPhysicsMovement) (Math|Vector|GetMaxElement (Math|Vector|MakeVector _hunter_2 _prey_2 _neutre_2)))
  (AI|Settings|SetDetectionRange (.detectioncreaturerangem BehaviorSettings))
  (Components|Sphere|SetSphereRadius _root (* (Variables|/Script/Engine.SphereComponent|GetSphereRadius _root) SizeToScale) true)
  (Default|Initialize (Variables|Default|GetBPC_StateManager_Movement) _detectmovementlist)
  (Default|Initialize (Variables|Default|GetBPC_StateManager_Detection) _detectstatelist)
  (Default|Initialize (Variables|Default|GetBPC_StateManager_Skills) _skillstatelist))

(fn SetMesh
  (params (Mesh :type Skeletal%20Mesh%20Object%20Reference) (Size :type Float%20%28double-precision%29))
  (bind _bpc_paramsbystring (Variables|Default|GetBPC_ParamsByString))
  (bind _skm_creature (Variables|Default|GetSKM_Creature))
  (if (Default|DoesParamExist _bpc_paramsbystring "SKM_Size")
    (LocalVariables|SetCurrentSKMSizeMultiplier (Default|GetValuebyParamName _bpc_paramsbystring "SKM_Size")))
  (Components|SkeletalMesh|SetSkeletalMeshAsset _skm_creature Mesh)
  (Transformation|SetWorldScale3D _skm_creature (* (* (LocalVariables|GetCurrentSKMSizeMultiplier) Size) (Transformation|GetWorldScale _skm_creature))))

(fn SetandBindComponents
  (bind _userdata (Variables|Data|GetUserData))
  (bind _userdata_2 (Variables|Data|GetUserData))
  (bind (_creaturesizetype _creaturebehaviorsettings) (Utilities|Struct|BreakS_CreatureDetailsInstanced _userdata))
  (bind (_creaturesizetype_2 _creaturebehaviorsettings_2) (Utilities|Struct|BreakS_CreatureDetailsInstanced _userdata_2))
  (Default|Initialize (Variables|Default|GetBPC_Prey) (Variables|Default|GetDetectionArea) _creaturesizetype_2 (.y (Utilities|Struct|BreakS_AICreatureBehaviorSettings _creaturebehaviorsettings_2)))
  (Default|Initialize (Variables|Default|GetBPC_Predator) (Variables|Default|GetDetectionArea) (.y (Utilities|Struct|BreakS_AICreatureBehaviorSettings _creaturebehaviorsettings)) _creaturesizetype))

(fn GetCreatureSize
  (bind _data (CallFunction|IGetCreatureData))
  (return (.creaturesizetype _data)))

(fn CanMoveForward
  (return (RaycastDirection|CanMovetoDirection (Transformation|GetActorForwardVector) (Utilities|Struct|BreakS_AICreatureBehaviorSettings (Data|GetAIData)))))

(fn SetFreeDirectiontoMove
  (params (ConeAngle :type Float%20%28double-precision%29) (Direction :type Vector))
  (bind (_output _hasadirection) (CallFunction|GetOneDirectionfromFirstConeNoHit 8 (+ (Transformation|GetActorLocation) (* (Transformation|GetActorForwardVector) (Variables|/Script/Engine.SphereComponent|GetSphereRadius (Variables|Default|GetRoot)))) Direction ConeAngle (* (Utilities|Struct|BreakS_AICreatureBehaviorSettings (Data|GetAIData)) 1.5) "TraceTypeQuery3" "None" 0.0 "(R=0.945328,G=0.045013,B=1.000000,A=1.000000)" (Variables|Default|GetActorsIgnoredToSee)))
  (if _hasadirection
    (Default|AddDirection (Variables|Default|GetBPC_ActorPhysicsMovement) (* _output 1e+01)))
  (return))

(fn SpawnSomething
  (params (Class :type Actor%20Class%20Reference) (SpawnTransform :type Transform))
  (LocalVariables|SetTransformToSpawn SpawnTransform)
  (bind (_outhit _returnvalue) (Collision|LineTraceByChannel (Transformation|GetActorLocation) (.Location (Math|Transform|BreakTransform SpawnTransform)) "TraceTypeQuery3" false 0 "None"))
  (if _returnvalue
    (LocalVariables|SetTransformToSpawn (Math|Transform|MakeTransform (- (.ImpactPoint (Collision|BreakHitResult _outhit)) (* (Transformation|GetActorForwardVector) 1e+03)) (.rotation (LocalVariables|GetTransformToSpawn)) (.scale (LocalVariables|GetTransformToSpawn)))))
  (bind _returnvalue_2 (Game|SpawnActorfromClass Class (LocalVariables|GetTransformToSpawn) "Undefined" "MultiplyWithRoot" 0 0))
  (return _returnvalue_2))

(fn SetIsCatcheable
  (params (Is%20Catcheable :type Boolean))
  (LocalVariables|SetPreviousValue (Variables|Default|GetIs%20Catcheable))
  (Variables|Default|SetIs%20Catcheable Is%20Catcheable)
  (if (!= (LocalVariables|GetPreviousValue) (Variables|Default|GetIs%20Catcheable))
    (if (Variables|Default|GetIs%20Catcheable)
      (CallFunction|BecomeCatcheableEvent)
      (else
        (CallFunction|BecomeNotCatcheableEvent)))))

(fn Activate
  (params (Active :type Boolean))
  (for _array_element (Components|GetChildrenComponents (Variables|Default|GetRoot) true)
    (Components|Activation|SetActive _array_element Active false))
  (Variables|/Script/Engine.PrimitiveComponent|SetbGenerateOverlapEvents (Variables|Default|GetRoot) Active)
  (Variables|/Script/Engine.PrimitiveComponent|SetbGenerateOverlapEvents (Variables|Default|GetDetectionArea) Active)
  (Variables|/Script/Engine.PrimitiveComponent|SetbGenerateOverlapEvents (Variables|Default|GetSKM_Creature) Active)
  (Components|Activation|SetActive (Variables|Default|GetBPC_ActorPhysicsMovement) Active false)
  (Components|Activation|SetActive (Variables|Default|GetBPC_StateManager_Movement) Active false)
  (Components|Activation|SetActive (Variables|Default|GetBPC_StateManager_Detection) Active false)
  (Components|Activation|SetActive (Variables|Default|GetBPC_StateManager_Skills) Active false)
  (Default|CallEDonComponentActive (Variables|Default|GetBPC_Prey) Active)
  (Default|CallEDonComponentActive (Variables|Default|GetBPC_Predator) Active)
  (Rendering|SetVisibility (Variables|Default|GetRoot) Active true))

(fn IsQuiet
  (return (Math|Boolean|NORBoolean (Default|HasPredatorinRange (Variables|Default|GetBPC_Prey)) (Default|HasPreyinRange (Variables|Default|GetBPC_Predator)))))

(fn GetDirectionAfterHitAround
  (params (Direction :type Vector) (CrossDirection :type Vector) (ConeAngle :type Float%20%28double-precision%29) (Range :type Float%20%28double-precision%29) (RadiusToCover :type Integer))
  (LocalVariables|SetNextDirection Direction)
  (bind (_nearesthit _hasahit) (CallFunction|GetNearestHitLocationfromSphereRadius :Origin (Transformation|GetActorLocation) :Direction Direction :CrossDirection CrossDirection :ConeAngle ConeAngle :Range Range :RadiusToCover RadiusToCover :ActorsToIgnore (Variables|Default|GetActorsIgnoredToSee)))
  (if _hasahit
    (LocalVariables|SetNextDirection (Math|Vector|GetUnitDirection(Vector) (Transformation|GetActorLocation) (.Location (Collision|BreakHitResult _nearesthit)))))
  (return (LocalVariables|GetNextDirection)))

(fn GetGreatestPercentDetection
  (params (S_AICreatureStates :type S%20AI%20Creature%20States%20Structure%20%28by%20ref%29))
  (bind (_detectmovementlist _detectstatelist _skillstatelist) (Utilities|Struct|BreakS_AICreatureStates S_AICreatureStates))
  (bind _currentarray (LocalVariables|GetCurrentArray))
  (bind _values (Utilities|Map|Values _detectmovementlist))
  (Utilities|Array|AppendArray _values (LocalVariables|GetCurrentArray))
  (bind _values_2 (Utilities|Map|Values _detectstatelist))
  (Utilities|Array|AppendArray _values_2 (LocalVariables|GetCurrentArray))
  (bind _values_3 (Utilities|Map|Values _skillstatelist))
  (Utilities|Array|AppendArray _values_3 _currentarray)
  (for _array_element _currentarray
    (LocalVariables|SetGreatestDistance (Math|Float|Max(Float) (LocalVariables|GetGreatestDistance) (Utilities|Struct|BreakS_StateCooldown _array_element))))
  (return (LocalVariables|GetGreatestDistance)))

(fn CreateSphere
  (params (InSphereRadius :type Float%20%28single-precision%29) (NewHidden :type Boolean) (CollisionProfileName :type Name :default "NoCollision"))
  (bind _returnvalue (AddComponent|AddSphereComponent true))
  (Components|Sphere|SetSphereRadius _returnvalue InSphereRadius true)
  (Development|SetHiddeninGame _returnvalue NewHidden false)
  (Rendering|SetVisibility _returnvalue true false)
  (Class|ShapeComponent|SetLineThickness _returnvalue 5e+01)
  (Collision|SetCollisionProfileName _returnvalue CollisionProfileName true :!class /Script/Engine.PrimitiveComponent)
  (return _returnvalue))

(fn CanMovetoDirection
  (params (Direction :type Vector) (Range :type Float%20%28double-precision%29))
  (bind _returnvalue (Transformation|GetActorLocation))
  (bind _bpc_actorphysicsmovement (Variables|Default|GetBPC_ActorPhysicsMovement))
  (bind _targettempspeed (Variables|Default|GetTargetTempSpeed))
  (bind (_outhit _returnvalue_2) (Collision|SphereTraceByChannel _returnvalue (+ _returnvalue (* Direction Range)) (Variables|/Script/Engine.SphereComponent|GetSphereRadius (Variables|Default|GetRoot)) "TraceTypeQuery3" false (Variables|Default|GetActorsIgnoredToSee) "None" true "(R=0.183238,G=1.000000,B=0.288692,A=1.000000)" "(R=0.105076,G=0.251329,B=1.000000,A=1.000000)" 0.0))
  (if _returnvalue_2
    (Variables|/Game/Blueprints/AddOn/Components/BPC_ActorPhysicsMovement.BPC_ActorPhysicsMovement_C|SetTargetSpeed _bpc_actorphysicsmovement (* (Math|Float|NormalizetoRange (Math|Vector|Distance(Vector) (.TraceStart (Collision|BreakHitResult _outhit)) (.ImpactPoint (Collision|BreakHitResult _outhit))) 0.0 (Math|Vector|Distance(Vector) (.TraceStart (Collision|BreakHitResult _outhit)) (.TraceEnd (Collision|BreakHitResult _outhit)))) _targettempspeed))
    (else
      (Variables|/Game/Blueprints/AddOn/Components/BPC_ActorPhysicsMovement.BPC_ActorPhysicsMovement_C|SetTargetSpeed _bpc_actorphysicsmovement _targettempspeed)))
  (return (not _returnvalue_2)))

(fn CreateStaticMesh
  (params (Static%20Mesh :type Static%20Mesh%20Object%20Reference) (Material :type Material%20Instance%20Object%20Reference) (Scale :type Float%20%28single-precision%29) (Rotation :type Rotator) (Offset :type Vector))
  (bind _returnvalue (AddComponent|AddStaticMeshComponent false (Math|Transform|MakeTransform Offset Rotation (* Scale "1.000000,1.000000,1.000000"))))
  (Components|StaticMesh|SetStaticMesh _returnvalue Static%20Mesh)
  (Rendering|Material|SetMaterial _returnvalue 0 Material)
  (return _returnvalue))

(fn SpawnSomethingonSocket
  (params (Class :type Actor%20Class%20Reference) (TargetName :type String))
  (bind _skm_creature (Variables|Default|GetSKM_Creature))
  (for _array_element (CallFunction|GetSocketName TargetName (Transformation|GetAllSocketNames _skm_creature))
    (LocalVariables|SetTransformToSpawn (Transformation|GetSocketTransform _skm_creature _array_element "RTS_World"))
    (bind _returnvalue (Game|SpawnActorfromClass Class (Math|Transform|MakeTransform (.location (LocalVariables|GetTransformToSpawn)) (.rotation (LocalVariables|GetTransformToSpawn)) "1.000000,1.000000,1.000000") "AlwaysSpawn" "OverrideRootScale" 0 0))
    (Transformation|AttachComponentToComponent _returnvalue (Variables|Default|GetSKM_Creature) _array_element "SnapToTarget" "SnapToTarget" "KeepWorld" false)
    (Utilities|Array|Add (LocalVariables|GetActorSpawned) _returnvalue))
  (return (LocalVariables|GetActorSpawned)))

(fn GetBPGameInstance
  (Variables|Default|GetBPGameInstance
    (:then
      _)
    (:else
      (bind _asbp_game_instance (Utilities|Casting|CastToBP_GameInstance (Game|GetGameInstance)))
      (Variables|Default|SetBPGameInstance _asbp_game_instance)))
  (return (Variables|Default|GetBPGameInstance)))

(fn AddActortoIgnored
  (params (NewItem :type Actor%20Object%20Reference%20%28by%20ref%29))
  (Utilities|Array|AddUnique (Variables|Default|GetActorsIgnoredToSee) NewItem))

(fn RemoveActortoIgnored
  (params (NewItem :type Actor%20Object%20Reference%20%28by%20ref%29))
  (Utilities|Array|RemoveItem (Variables|Default|GetActorsIgnoredToSee) NewItem))

(fn GetSkeletalMesh
  (return (Utilities|ResolveSoftReference (Variables|Default|GetSKM_Creature))))

(fn IGetCreatureData
  (return (Variables|Data|GetUserData)))

(fn IGetMicroArea
  (return (Variables|Data|GetCurrentMicroArea)))

(fn IIsCatcheable
  (return (Variables|Default|GetIs%20Catcheable)))

(fn IIsinMicroArea
  (params (Target :type E_MicroZone%20Enum :default "NewEnumerator4"))
  (return (Utilities|Enum|Equal(Enum) Target (Variables|Data|GetCurrentMicroArea))))