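; Top-level manager that distance-culls every BP_CreatureManager in the level relative to the player.
; BeginPlay caches those managers and the game instance, calls IStart on each, then enables ticking.
; Each Tick, managers within the CullingManager distance are started or, if already active, updated with delta time, while active ones out of range are quit.
; Near and far states are printed as debug text.
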(event EventBeginPlay
  (bind _outactors (Actor|GetAllActorsOfClass "/Game/Blueprints/AI/Manager/BP_CreatureManager.BP_CreatureManager_C"))
  (Variables|Default|SetManagerList _outactors)
  (bind _asbp_game_instance (Utilities|Casting|CastToBP_GameInstance (Game|GetGameInstance)))
  (Variables|Default|SetGame%20Instance _asbp_game_instance)
  (for _array_element (Variables|Default|GetManagerList)
    (Default|IStart _array_element))
  (Actor|Tick|SetActorTickEnabled true))

(event EventTick
  (params (DeltaSeconds :type Float%20%28single-precision%29))
  (for _array_element (Variables|Default|GetManagerList)
    (if (CallFunction|GetMinimalDistance _array_element)
      (if (Variables|/Game/Blueprints/AI/Manager/BP_CreatureManager.BP_CreatureManager_C|GetIsActive _array_element)
        (Default|IUpdate _array_element DeltaSeconds)
        (Development|PrintText "Is Near" true true "(R=1.000000,G=0.000000,B=0.067612,A=1.000000)" 0.0)
        (else
          (Default|IStart _array_element)))
      (else
        (if (Variables|/Game/Blueprints/AI/Manager/BP_CreatureManager.BP_CreatureManager_C|GetIsActive _array_element)
          (Default|IQuit _array_element))
        (Development|PrintText "Is Far" true true "(R=0.105615,G=1.000000,B=0.000000,A=1.000000)" 0.0)))))

(fn ConstructionScript)

(fn GetMinimalDistance
  (params (Target :type Actor%20Object%20Reference))
  (return (<= (Math|Vector|Distance(Vector) (Transformation|GetActorLocation Target) (Transformation|GetActorLocation (Variables|/Game/Blueprints/Data/BP_GameInstance.BP_GameInstance_C|GetPlayer (Variables|Default|GetGame%20Instance)))) (Variables|Default|GetCullingManager))))