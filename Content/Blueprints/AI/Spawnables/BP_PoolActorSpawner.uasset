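; Spawner actor that periodically launches pooled actors of a configurable class at random points within its shape.
; On BeginPlay it requests a pool from the Play_Mode game mode by class and parameters, then starts a looping spawn timer.
; SpawnObject launches a pool actor with random rotation and unit scale, reusing pooled actors.
; It prints a message if the Play_Mode cast fails.
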(event Custom|SpawnObject
  (Default|LaunchPoolActor (Variables|Default|GetPool) (Math|Transform|MakeTransform (CallFunction|GetRandomPointinShape) (Math|Random|RandomRotator true))))

(event EventBeginPlay
  (bind _asplay_mode (Utilities|Casting|CastToPlay_Mode (Game|GetGameMode))
    (:then
      (bind _value (Default|TryGetPool _asplay_mode (Variables|Init|GetClassToSpawn) (Variables|/Game/Blueprints/AddOn/Components/GenericComponents/BPC_ParamsByString.BPC_ParamsByString_C|GetParams (Variables|Default|GetBPC_ParamsByString))))
      (Variables|Default|SetPool _value)
      (Utilities|Time|SetTimerbyEvent (EventDispatchers|CreateEvent :!event Custom|SpawnObject) (Variables|Init|GetSpawnTimer) true))
    (:CastFailed
      (Development|PrintText "Game Mode Don't Exist" true true "(R=1.000000,G=0.042729,B=0.000000,A=1.000000)" 3.0))))

(fn ConstructionScript
  (|CallParentFunction))