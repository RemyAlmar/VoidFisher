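; BP_Bubble is a pooled bubble hazard that slows actors with BPC_ActorPhysicsMovement while they overlap it.
; Leaving the pool randomizes size from string-keyed params, plays scale and drift timelines, and starts a lifetime timer.
; Tick runs only with tracked occupants, reducing their TargetSpeed.
; Larger bubbles absorb smaller ones and grow; exiting occupants or reaching the size cap pop it back into the pool with Niagara and sound.
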(event OnComponentBeginOverlap(SphereCollision)
  (params (OverlappedComponent :type Primitive%20Component%20Object%20Reference) (OtherActor :type Actor%20Object%20Reference) (OtherComp :type Primitive%20Component%20Object%20Reference) (OtherBodyIndex :type Integer) (bFromSweep :type Boolean) (SweepResult :type Hit%20Result%20Structure%20%28by%20ref%29))
  (bind _returnvalue (Actor|GetComponentbyClass OtherActor "/Game/Blueprints/AddOn/Components/BPC_ActorPhysicsMovement.BPC_ActorPhysicsMovement_C"))
  (bind _size (Variables|Data|GetSize))
  (Utilities|IsValid _returnvalue
    (:Is%20Valid
      (Utilities|Array|AddUnique (Variables|Default|GetPhysicsComponents) _returnvalue)
      (Audio|PlaySound2D "/Game/SFX/Sounds/NEW_OGG/Menu_UI_UX/Menu/SoundWave/SFX_ButtonHoveredMenu.SFX_ButtonHoveredMenu" 1.0 1.0 0.0 0 0 false) ; Allo faut l'atteniuation les gens!!!
      (Actor|Tick|SetActorTickEnabled (Utilities|Array|IsNotEmpty (Variables|Default|GetPhysicsComponents))))
    (:Is%20Not%20Valid
      (bind _asbp_bubble (Utilities|Casting|CastToBP_Bubble OtherActor))
      (Utilities|IsValid _asbp_bubble
        (:Is%20Valid
          (if (> _size (Variables|BP_Bubble_C|GetSize _asbp_bubble))
            (Default|EDBacktoPoolEvent _asbp_bubble)
            (CallFunction|ChangeSize _size (+ _size (Variables|BP_Bubble_C|GetSize _asbp_bubble)))))))))

(event OnComponentEndOverlap(SphereCollision)
  (params (OverlappedComponent :type Primitive%20Component%20Object%20Reference) (OtherActor :type Actor%20Object%20Reference) (OtherComp :type Primitive%20Component%20Object%20Reference) (OtherBodyIndex :type Integer))
  (bind _returnvalue (Actor|GetComponentbyClass OtherActor "/Game/Blueprints/AddOn/Components/BPC_ActorPhysicsMovement.BPC_ActorPhysicsMovement_C"))
  (Utilities|IsValid _returnvalue
    (:Is%20Valid
      (if (Utilities|Array|ContainsItem (Variables|Default|GetPhysicsComponents) _returnvalue)
        (CallFunction|EDBacktoPoolEvent)))))

(event Custom|MoveAnim
  (bind _moveto (Timeline|Move PlayFromStart)
    (:Update
      (Transformation|AddActorWorldOffset (* (Variables|Default|GetTargetLocation) _moveto)))))

(event Custom|OnDisplay
  (bind _scale (Timeline|Appear PlayFromStart)
    (:Update
      (Transformation|SetActorScale3D (Math|Conversions|ToVector(Float) _scale)))
    (:Finished
      (CallFunction|ActiveActor true))))

(event Custom|BubbleExplode
  (Niagara|SpawnSystematLocation "/Game/VFX/Niagara/Environment/Bubbles/NS_BubbleExplosed.NS_BubbleExplosed" (Transformation|GetActorLocation) (Transformation|GetActorRotation) "1.000000,1.000000,1.000000" true true "AutoRelease")
  (Audio|PlaySound2D "/Game/SFX/Sounds/PLACEHOLDER/BubblePop.BubblePop" 1.0 1.0 0.0 0 0 false) ; Allo faut l'atteniuation les gens!!!
)

(event Custom|ChangeSize
  (params (PreviousSize :type Float%20%28double-precision%29) (TargetSize :type Float%20%28double-precision%29))
  (bind _size (Timeline|Timeline PlayFromStart)
    (:Update
      (CallFunction|SetSize (Math|Float|Lerp PreviousSize TargetSize _size)))
    (:Finished
      (if (>= (Variables|Data|GetSize) 3e+02)
        (CallFunction|EDBacktoPoolEvent)))))

(event EventTick
  (params (DeltaSeconds :type Float%20%28single-precision%29))
  (for _array_element (Variables|Default|GetPhysicsComponents)
    (Variables|/Game/Blueprints/AddOn/Components/BPC_ActorPhysicsMovement.BPC_ActorPhysicsMovement_C|SetTargetSpeed _array_element (- (Variables|/Game/Blueprints/AddOn/Components/BPC_ActorPhysicsMovement.BPC_ActorPhysicsMovement_C|GetTargetSpeed _array_element) (* (Utilities|GetPercentSlowdown) (* (Variables|/Game/Blueprints/AddOn/Components/BPC_ActorPhysicsMovement.BPC_ActorPhysicsMovement_C|GetTargetSpeed _array_element) 0.1))))))

(event EventEDCometoPoolEvent
  (bind _bpc_paramsbystring (Variables|Default|GetBPC_ParamsByString))
  (CallFunction|SetSize (Math|Random|RandomFloatinRange (Default|GetParambyName _bpc_paramsbystring "SizeMin") (Default|GetParambyName _bpc_paramsbystring "SizeMax")))
  (|CallParentFunction)
  (Variables|Default|SetTargetLocation (* (Math|Random|RandomUnitVector) (Math|Random|RandomFloatinRange 2.0 15.0)))
  (CallFunction|OnDisplay)
  (CallFunction|MoveAnim)
  (CallFunction|ActiveRenderer true)
  (Utilities|Time|SetTimerbyEvent (EventDispatchers|CreateEvent :!event EDBacktoPoolEvent) (Default|GetParambyName (Variables|Default|GetBPC_ParamsByString) "TimeBeforeDestroy")))

(event EventEDBacktoPoolEvent
  (bind _bpc_paramsbystring (Variables|Default|GetBPC_ParamsByString))
  (CallFunction|BubbleExplode)
  (CallFunction|ActiveActor false)
  (CallFunction|SetSize (Math|Random|RandomFloatinRange (Default|GetParambyName _bpc_paramsbystring "SizeMin") (Default|GetParambyName _bpc_paramsbystring "SizeMax")))
  (|CallParentFunction))

(fn ConstructionScript)

(fn ActiveActor
  (params (Active :type Boolean))
  (Utilities|Array|Clear (Variables|Default|GetPhysicsComponents))
  (Variables|/Script/Engine.PrimitiveComponent|SetbGenerateOverlapEvents (Variables|Default|GetSphereCollision) Active)
  (Rendering|SetVisibility (Variables|Default|GetSphere) Active false)
  (Actor|Tick|SetActorTickEnabled (Utilities|Array|IsNotEmpty (Variables|Default|GetPhysicsComponents)))
  (return))

(fn SetSize
  (params (Size :type Float%20%28double-precision%29))
  (Variables|Data|SetSize Size)
  (Components|Sphere|SetSphereRadius (Variables|Default|GetSphereCollision) (* (Variables|Data|GetSize) (Variables|CONST|GetBaseSphereRadius)) true)
  (Transformation|SetWorldScale3D (Variables|Default|GetSphere) (Math|Conversions|ToVector(Float) (Variables|Data|GetSize))))

(fn ActiveRenderer
  (params (Active :type Boolean))
  (Rendering|SetVisibility (Variables|Default|GetSphere) Active false)
  (return))

(fn ActiveCollisions
  (params (Active :type Boolean))
  (Utilities|Array|Clear (Variables|Default|GetPhysicsComponents))
  (Variables|/Script/Engine.PrimitiveComponent|SetbGenerateOverlapEvents (Variables|Default|GetSphereCollision) Active)
  (Actor|Tick|SetActorTickEnabled (Utilities|Array|IsNotEmpty (Variables|Default|GetPhysicsComponents)))
  (return))