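; BP_Node is a pathfinding node for AI that stores a parent node, a location and a path cost.
; Initialize sets the parent and location, then sets CurrentPathCost to the parent's distance from its own parent plus this node's distance from the parent.
; The cost therefore spans only the last two links, as it does not read the parent's accumulated CurrentPathCost.
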(fn GetDistancefromParentNode
  (bind _parentnode (Variables|Default|GetParentNode))
  (Utilities|IsValid _parentnode
    (:Is%20Valid
      (return (Math|Vector|Distance(Vector) (Variables|BP_Node_C|GetLocation _parentnode) (Variables|Default|GetLocation))))))

(fn Initialize
  (params (ParentNode :type BP%20Node%20Object%20Reference) (Location :type Vector))
  (Variables|Default|SetParentNode ParentNode)
  (Variables|Default|SetLocation Location)
  (Variables|Default|SetCurrentPathCost (+ (Node|Distance|GetDistancefromParentNode ParentNode) (Node|Distance|GetDistancefromParentNode))))