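; Pathfinding component, still in progress, that probes ahead of its owning actor and sketches a node-based path search.
; Each Tick fires a debug-drawn forward line trace plus a cone trace, with results unused.
; FindPath, not called here, picks the cheapest open BP_Node and retraces parent links at the goal.
; The search never expands neighbours or removes nodes, so it loops endlessly unless the start is within tolerance.
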(event EventTick
  (params (DeltaSeconds :type Float%20%28single-precision%29))
  (CallFunction|CreateDetectRay))

(fn FindPath
  (params (StartPos :type Vector) (GoalPos :type Vector))
  (bind _openlist (LocalVariables|GetOpenList))
  (bind _returnvalue (HandlerNode|CreateNode 0 StartPos))
  (Utilities|Array|Add (LocalVariables|GetOpenList) _returnvalue)
  (while (> (Utilities|Array|Length _openlist) 0)
    (bind _output_get (LocalVariables|SetCurrentNode (HandlerNode|GetLowestCostNode _openlist)))
    (if (Utilities|Operators|EqualEqual (Variables|/Game/Blueprints/AI/Pathfinding/BP_Node.BP_Node_C|GetLocation _output_get) GoalPos (Variables|Path|GetRadiusTolerance))
      (bind _pathvalues (Path|RetracePath (LocalVariables|GetCurrentNode)))
      (return _pathvalues))))

(fn CreateNode
  (params (ParentNode :type BP%20Node%20Object%20Reference) (Location :type Vector))
  (bind _returnvalue (Game|ConstructObjectfromClass "/Game/Blueprints/AI/Pathfinding/BP_Node.BP_Node_C"))
  (Default|Initialize _returnvalue ParentNode Location)
  (return _returnvalue))

(fn GetLowestCostNode
  (params (NodeList :type Array%20of%20BP%20Node%20Object%20References))
  (LocalVariables|SetNodeLowCost (Utilities|Array|Get(acopy) NodeList))
  (for _array_element NodeList
    (if (< (Variables|/Game/Blueprints/AI/Pathfinding/BP_Node.BP_Node_C|GetCurrentPathCost _array_element) (Variables|/Game/Blueprints/AI/Pathfinding/BP_Node.BP_Node_C|GetCurrentPathCost (LocalVariables|GetNodeLowCost)))
      (LocalVariables|SetNodeLowCost _array_element)))
  (return (LocalVariables|GetNodeLowCost)))

(fn RetracePath
  (params (TargetNode :type BP%20Node%20Object%20Reference))
  (bind _path (LocalVariables|GetPath))
  (LocalVariables|SetCurrentNode TargetNode)
  (while (!= (Variables|/Game/Blueprints/AI/Pathfinding/BP_Node.BP_Node_C|GetParentNode (LocalVariables|GetCurrentNode)) 0)
    (Utilities|Array|Add (LocalVariables|GetPath) (Variables|/Game/Blueprints/AI/Pathfinding/BP_Node.BP_Node_C|GetLocation (LocalVariables|GetCurrentNode)))
    (LocalVariables|SetCurrentNode (Variables|/Game/Blueprints/AI/Pathfinding/BP_Node.BP_Node_C|GetParentNode (LocalVariables|GetCurrentNode))))
  (Utilities|Array|Reverse _path)
  (return _path))

(fn CreateDetectRay
  (bind _returnvalue (Components|GetOwner))
  (bind _returnvalue_2 (Transformation|GetActorLocation _returnvalue))
  (bind _returnvalue_3 (Transformation|GetActorForwardVector _returnvalue))
  (Collision|LineTraceByChannel _returnvalue_2 (+ _returnvalue_2 (* _returnvalue_3 (Variables|Raycast|GetRayLength))) "TraceTypeQuery1" false 0 "Persistent" true "(R=0.891247,G=1.000000,B=0.969732,A=1.000000)" "(R=1.000000,G=0.086574,B=0.000000,A=1.000000)" 0.1)
  (CallFunction|ConeTracebyChannel (Variables|Path|GetRayNumber) _returnvalue_2 _returnvalue_3 (Variables|Raycast|GetConeAngle) (Variables|Raycast|GetRayLength)))