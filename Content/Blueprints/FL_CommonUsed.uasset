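; Blueprint function library of shared math helpers for sign extraction, timers and time-driven value changes.
; TimerPos and TimerNeg advance a by-ref time up or down, clamp or auto-reset at the limit, and return whether it was hit.
; IncreaseValueInTime and DecreaseValueInTime use those timers to scale a by-ref value linearly with elapsed time, clamped between zero and its max.
; IncreaseValueExp adds an input-scaled power term, also clamped.
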(fn GetSignedValue
  (params (Value :type Float%20%28double-precision%29))
  (return (/ Value (Math|Float|Absolute(Float) Value))))

(fn TimerPos
  (params (CurrentTime :type Float%20%28double-precision%29%20%28by%20ref%29) (MaxTime :type Float%20%28double-precision%29) (DeltaTime :type Float%20%28double-precision%29) (AutoResetTimer :type Boolean))
  (bind _output_get (LocalVariables|SetFutureTime (+ CurrentTime (Math|Float|Absolute(Float) DeltaTime))))
  (bind _output_get_2 (LocalVariables|SetTimeReached (>= _output_get MaxTime)))
  (if _output_get_2
    (if AutoResetTimer
      (LocalVariables|SetFutureTime 0.0)
      (else
        (LocalVariables|SetFutureTime MaxTime))))
  (|SetBy-RefVar CurrentTime (LocalVariables|GetFutureTime))
  (return (LocalVariables|GetTimeReached)))

(fn TimerNeg
  (params (CurrentTime :type Float%20%28double-precision%29%20%28by%20ref%29) (TimeMax :type Float%20%28double-precision%29) (DeltaTime :type Float%20%28double-precision%29) (AutoResetTimer :type Boolean))
  (LocalVariables|SetFutureTime (- CurrentTime (Math|Float|Absolute(Float) DeltaTime)))
  (bind _output_get (LocalVariables|SetTimeSpended (<= (LocalVariables|GetFutureTime) 0.0)))
  (if _output_get
    (if AutoResetTimer
      (LocalVariables|SetFutureTime TimeMax)
      (else
        (LocalVariables|SetFutureTime 0.0))))
  (|SetBy-RefVar CurrentTime (LocalVariables|GetFutureTime))
  (return (LocalVariables|GetTimeSpended)))

(fn IncreaseValueinTime
  (params (ValueToIncrease :type Float%20%28double-precision%29%20%28by%20ref%29) (CurrentTime :type Float%20%28double-precision%29%20%28by%20ref%29) (DeltaTime :type Float%20%28double-precision%29) (SpeedMultiplierToIncrease :type Float%20%28double-precision%29) (ValueMax :type Float%20%28double-precision%29) (TimeMax :type Float%20%28double-precision%29) (AutoResetTimer :type Boolean))
  (if (Timer|TimerPos CurrentTime TimeMax (* DeltaTime SpeedMultiplierToIncrease) AutoResetTimer)
    (|SetBy-RefVar ValueToIncrease ValueMax)
    (else
      (|SetBy-RefVar ValueToIncrease (* ValueMax (Math|Float|NormalizetoRange (Math|Float|Lerp 0.0 TimeMax (/ CurrentTime TimeMax)) 0.0 TimeMax)))))
  (|SetBy-RefVar ValueToIncrease (Math|Float|Clamp(Float) ValueToIncrease 0.0 ValueMax))
  (return ValueToIncrease))

(fn DecreaseValueinTime
  (params (ValueToDecreased :type Float%20%28double-precision%29%20%28by%20ref%29) (CurrentTime :type Float%20%28double-precision%29%20%28by%20ref%29) (DeltaTime :type Float%20%28double-precision%29) (SpeedMutliplierToDecrease :type Float%20%28double-precision%29) (TimeMax :type Float%20%28double-precision%29) (ValueMax :type Float%20%28double-precision%29) (AutoResetTimer :type Boolean))
  (if (Timer|TimerNeg CurrentTime TimeMax (* DeltaTime SpeedMutliplierToDecrease) AutoResetTimer)
    _
    (else
      _))
  (|SetBy-RefVar ValueToDecreased (* ValueMax (Math|Float|NormalizetoRange (Math|Float|Lerp 0.0 TimeMax (/ CurrentTime TimeMax)) 0.0 TimeMax)))
  (|SetBy-RefVar ValueToDecreased (Math|Float|Clamp(Float) ValueToDecreased 0.0 ValueMax))
  (return ValueToDecreased))

(fn IncreaseValueExp
  (params (ValueToIncrease :type Float%20%28double-precision%29%20%28by%20ref%29) (InputValue :type Float%20%28double-precision%29) (ValueToAdd :type Float%20%28double-precision%29) (Exp :type Float%20%28double-precision%29) (ClampValueMax :type Float%20%28double-precision%29))
  (|SetBy-RefVar ValueToIncrease (Math|Float|Clamp(Float) (+ ValueToIncrease (* InputValue (Math|Float|Power ValueToAdd Exp))) 0.0 ClampValueMax))
  (return))