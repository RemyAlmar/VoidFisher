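; BP_SkeletalFoliage is a skeletal-mesh foliage actor, apparently a test of physics-driven plants through the Physics Control component.
; On BeginPlay it builds world- and parent-space controls and kinematic, zero-gravity, physics-only body modifiers from limb bones.
; It copies the "WorldSpace_Sea" controls into "WorldSpace_SeaAll" and sets their linear and angular strengths.
; It also requests kinematic movement using that set's name as a single modifier name.
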(event EventBeginPlay
  (bind _physicscontrol (Variables|Default|GetPhysicsControl))
  (bind _physicscontrol_2 (Variables|Default|GetPhysicsControl))
  (Class|PhysicsControlComponent|CreateControlsandBodyModifiersfromLimbBones (Variables|Default|GetPhysicsControl) (Variables|Default|GetSkeletalMesh) (Variables|Default|GetLimb%20Setup%20Data) (Variables|Default|GetWorld%20Space%20Control%20Data) (Variables|Default|GetParent%20Space%20Control%20Data) (Utilities|Struct|MakePhysicsControlModifierData "Kinematic" "PhysicsOnly" 0.0 1.0 true true) 0 "None")
  (Utilities|FlowControl|Sequence
    (:then_0
      (Class|PhysicsControlComponent|AddControlstoSet _physicscontrol (Class|PhysicsControlComponent|GetControlNamesinSet _physicscontrol "WorldSpace_Sea") "WorldSpace_SeaAll"))
    (:then_1
      (Class|PhysicsControlComponent|SetBodyModifierMovementType _physicscontrol_2 "WorldSpace_SeaAll" "Kinematic")
      (Class|PhysicsControlComponent|SetControlDatasinSet _physicscontrol_2 "WorldSpace_SeaAll" (Utilities|Struct|MakePhysicsControlData 1.0 1.0 0.0 0.0 1.0 1.0 0.0 0.0 1.0 1.0 1.0 "0.000000,0.000000,0.000000" true false true false false)))))

(fn ConstructionScript)