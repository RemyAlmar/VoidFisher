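; BP_Torus is an environment torus prop that spins continuously and carries randomly scattered plants.
; The construction script applies the configurable root mesh to the torus.
; BeginPlay randomises the spin speed, then repeatedly reveals random child components and assigns random plant meshes through separate random picks, within a count capped by the child total.
; Tick adds local yaw by that speed each frame, without delta-time scaling.
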(event EventBeginPlay
  (bind _torus (Variables|Default|GetTorus))
  (bind _plantminmax (Variables|Param|Render|GetPlantMinMax))
  (bind _children (Components|GetChildrenComponents _torus false))
  (bind _outitem (Utilities|Array|Random _children))
  (Variables|Param|Speed|SetSpeedRate (CallFunction|GetRandomFloatwithGap 0.1 (Variables|Param|Speed|GetSpeedRate)))
  (for _index (range 0 (Math|Integer|Clamp(Integer) (Math|Random|RandomIntegerinRange (.min _plantminmax) (.max _plantminmax)) 0 (Utilities|Array|LastIndex _children)))
    (Rendering|SetVisibility _outitem true false)
    (bind _asstatic_mesh_component (Utilities|Casting|CastToStaticMeshComponent _outitem))
    (Components|StaticMesh|SetStaticMesh _asstatic_mesh_component (.OutItem (Utilities|Array|Random (Variables|Param|Render|GetPlant_SM))))))

(event EventTick
  (params (DeltaSeconds :type Float%20%28single-precision%29))
  ;[1 0.3229 0.3229] Le torus il touuuuuuurneeeeeeeeeeeeeeeeeeeeeeeeeeeeeeeeeeeeeeeeeeeeeeeeeeeeeeeeeeeeeeeeeeeeeeeeeeeeeeeeeeeeeeeeeeeeeeeeeeeeeeeeeeeeeeeeeeeeeeeeeeeeeeeeeeeeeeeeeeeeeeeeeeeeeeeeeeeeeeeeeeeeeeeeeeeeeeeeeeeeeeeeeeeeeeeeeeeeeeeeeeeeeeeeeeeeeeeeeeeeeeeeeeeeeeeeeeeeeeeeeeeeeeeeeeeeeeeeeee
  (Transformation|AddLocalRotation (Variables|Default|GetTorus) (Math|Rotator|MakeRotator 0.0 0.0 (Variables|Param|Speed|GetSpeedRate)) false false))

(fn ConstructionScript
  (Components|StaticMesh|SetStaticMesh (Variables|Default|GetTorus) (Variables|Param|Render|GetRoot_SM)))